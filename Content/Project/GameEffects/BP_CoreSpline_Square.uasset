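; BP_CoreSpline_Square is a game effect Blueprint that moves a small Runner component along a spline.
; On BeginPlay it calls the parent, then plays a timeline whose AnimTest track, scaled by spline length, gives the distance along the spline.
; Each update sets the Runner's relative transform from the spline's local location and rotation at that distance, with a fixed small scale.
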(event EventBeginPlay
  (bind _spline (Variables|Default|GetSpline))
  (|CallParentFunction)
  (bind _animtest (Timeline|Timeline PlayFromStart)
    (:Update
      (Transformation|SetRelativeTransform (Variables|Default|GetRunner) (Math|Transform|MakeTransform (Spline|GetLocationatDistanceAlongSpline _spline (* _animtest (Spline|GetSplineLength _spline)) "Local") (Spline|GetRotationatDistanceAlongSpline _spline (* _animtest (Spline|GetSplineLength _spline)) "Local") "0.025000,0.025000,0.025000") false false))))

(fn ConstructionScript
  (|CallParentFunction))