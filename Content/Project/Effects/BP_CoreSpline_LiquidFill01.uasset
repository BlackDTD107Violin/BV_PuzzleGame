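; BP_CoreSpline_LiquidFill01 is an effect actor that moves two small runner components along two splines.
; On BeginPlay a timeline starts, and its AnimTest track gives the normalized distance, scaled by each spline's length.
; Each update sets Runner and Runner1 to the local location and rotation at that distance on Spline and Spline1, with a fixed small scale.
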(event EventBeginPlay
  (bind _spline (Variables|Default|GetSpline))
  (bind _spline1 (Variables|Default|GetSpline1))
  (|CallParentFunction)
  (bind _animtest (Timeline|Timeline PlayFromStart)
    (:Update
      (Variables|Default|SetAnim%20Test _animtest)
      (Utilities|FlowControl|Sequence
        (:then_0
          (Transformation|SetRelativeTransform (Variables|Default|GetRunner) (Math|Transform|MakeTransform (Spline|GetLocationatDistanceAlongSpline _spline (* (Variables|Default|GetAnim%20Test) (Spline|GetSplineLength _spline)) "Local") (Spline|GetRotationatDistanceAlongSpline _spline (* (Variables|Default|GetAnim%20Test) (Spline|GetSplineLength _spline)) "Local") "0.025000,0.025000,0.025000") false false))
        (:then_1
          (Transformation|SetRelativeTransform (Variables|Default|GetRunner1) (Math|Transform|MakeTransform (Spline|GetLocationatDistanceAlongSpline _spline1 (* (Variables|Default|GetAnim%20Test) (Spline|GetSplineLength _spline1)) "Local") (Spline|GetRotationatDistanceAlongSpline _spline1 (* (Variables|Default|GetAnim%20Test) (Spline|GetSplineLength _spline1)) "Local") "0.025000,0.025000,0.025000") false false))))))

(fn ConstructionScript
  (|CallParentFunction))