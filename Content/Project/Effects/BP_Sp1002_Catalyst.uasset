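; Catalyst effect actor that animates five small runner components along their own spline paths.
; On BeginPlay a timeline plays from the start, and its AnimTest value scales each spline's length into a distance along that spline.
; Each update sets every runner's relative transform to the local-space location and rotation at that distance, with a fixed tiny scale.
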(event EventBeginPlay
  (bind _spline3 (Variables|Default|GetSpline3))
  (bind _spline2 (Variables|Default|GetSpline2))
  (bind _spline4 (Variables|Default|GetSpline4))
  (bind _spline (Variables|Default|GetSpline))
  (bind _spline1 (Variables|Default|GetSpline1))
  (|CallParentFunction)
  (bind _animtest (Timeline|Timeline PlayFromStart)
    (:Update
      (Variables|Default|SetAnim%20Test _animtest)
      (Utilities|FlowControl|Sequence
        (:then_0
          (Transformation|SetRelativeTransform (Variables|Default|GetRunner) (Math|Transform|MakeTransform (Spline|GetLocationatDistanceAlongSpline _spline (* (Variables|Default|GetAnim%20Test) (Spline|GetSplineLength _spline)) "Local") (Spline|GetRotationatDistanceAlongSpline _spline (* (Variables|Default|GetAnim%20Test) (Spline|GetSplineLength _spline)) "Local") "0.025000,0.025000,0.025000") false false))
        (:then_1
          (Transformation|SetRelativeTransform (Variables|Default|GetRunner1) (Math|Transform|MakeTransform (Spline|GetLocationatDistanceAlongSpline _spline1 (* (Variables|Default|GetAnim%20Test) (Spline|GetSplineLength _spline1)) "Local") (Spline|GetRotationatDistanceAlongSpline _spline1 (* (Variables|Default|GetAnim%20Test) (Spline|GetSplineLength _spline1)) "Local") "0.025000,0.025000,0.025000") false false))
        (:then_2
          (Transformation|SetRelativeTransform (Variables|Default|GetRunner2) (Math|Transform|MakeTransform (Spline|GetLocationatDistanceAlongSpline _spline2 (* (Variables|Default|GetAnim%20Test) (Spline|GetSplineLength _spline2)) "Local") (Spline|GetRotationatDistanceAlongSpline _spline2 (* (Variables|Default|GetAnim%20Test) (Spline|GetSplineLength _spline2)) "Local") "0.025000,0.025000,0.025000") false false))
        (:then_3
          (Transformation|SetRelativeTransform (Variables|Default|GetRunner4) (Math|Transform|MakeTransform (Spline|GetLocationatDistanceAlongSpline _spline4 (* (Variables|Default|GetAnim%20Test) (Spline|GetSplineLength _spline4)) "Local") (Spline|GetRotationatDistanceAlongSpline _spline4 (* (Variables|Default|GetAnim%20Test) (Spline|GetSplineLength _spline4)) "Local") "0.025000,0.025000,0.025000") false false))
        (:then_4
          (Transformation|SetRelativeTransform (Variables|Default|GetRunner3) (Math|Transform|MakeTransform (Spline|GetLocationatDistanceAlongSpline _spline3 (* (Variables|Default|GetAnim%20Test) (Spline|GetSplineLength _spline3)) "Local") (Spline|GetRotationatDistanceAlongSpline _spline3 (* (Variables|Default|GetAnim%20Test) (Spline|GetSplineLength _spline3)) "Local") "0.025000,0.025000,0.025000") false false))))))

(fn ConstructionScript
  (|CallParentFunction))