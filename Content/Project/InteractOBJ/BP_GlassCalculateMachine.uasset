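; BP_GlassCalculateMachine is an interactable machine that routes GLASS codes through a collection panel and previews the glass totem.
; On BeginPlay it caches its panel and previewer child actors and sets the previewer's type.
; Its functions act as a facade: the panel distributes and collects codes, while the previewer receives the current GLASS and Distance, Expand, Rotate and Scaling spline updates.
; An older material-parameter preview path remains unconnected.
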(event EventBeginPlay
  (|CallParentFunction)
  (Utilities|FlowControl|Sequence
    (:then_0
      (bind _asbp_collection_machine_demo_beta (Utilities|Casting|CastToBP_CollectionMachineDemo_beta (Variables|/Script/Engine.ChildActorComponent|GetChildActor (Variables|Default|GetInteractPanel))))
      (Variables|Default|SetREF_Collection%20MachinePanel _asbp_collection_machine_demo_beta))
    (:then_1
      (bind _asbp_glass_totem_previewer (Utilities|Casting|CastToBP_GlassTotemPreviewer (Variables|/Script/Engine.ChildActorComponent|GetChildActor (Variables|Default|GetGlassPreview))))
      (bind _output_get (Variables|Default|SetREF_GlassPreviewer _asbp_glass_totem_previewer))
      (Variables|/Game/Project/InteractOBJ/BP_GlassTotemPreviewer.BP_GlassTotemPreviewer_C|SetTotemPreviewType _output_get "NewEnumerator3"))))

(fn ConstructionScript
  (|CallParentFunction))

(fn ReceiveGLASSCode
  (params (GLASSInserted :type ST%20Glass%20Base%20Collection%20Structure))
  (Default|AssignGLASSCodetoEachFunc (Variables|Default|GetREF_Collection%20MachinePanel) GLASSInserted))

(fn ReturnUpdatedGLASSCode
  (bind _updatedglass (Default|CollectGLASSCodefromEachFunc (Variables|Default|GetREF_Collection%20MachinePanel)))
  (return _updatedglass))

(fn UpdateTotemPreviewer
  (params (Distance :type Integer) (Expand :type Integer) (Rotate :type Integer) (Scaling :type Integer))
  (Default|UpdatePreviewerGLASSSpline (Variables|Default|GetREF_GlassPreviewer) Distance Expand Rotate Scaling))

(fn AssignTotemPreviewer
  (params (CurrentGLASS :type ST%20Glass%20Base%20Collection%20Structure))
  (Default|ReceiveGLASSPreviewer (Variables|Default|GetREF_GlassPreviewer) CurrentGLASS "NewEnumerator0" (Utilities|Array|Get(acopy) (Utilities|Struct|BreakST_GlassBaseCollection CurrentGLASS))))