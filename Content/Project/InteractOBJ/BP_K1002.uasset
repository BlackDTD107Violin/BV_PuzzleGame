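; BP_K1002 is an interactable wine bottle object that relies on its parent class for inspection and extraction-glow behavior.
; Its construction script creates dynamic material instances for the glass and cork slots and registers both in the extract component's material groups.
; The event graph only forwards begin play, inspector enter and exit, and extract glowing to the parent.
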(event EventBeginPlay
  (|CallParentFunction))

(event EventItemExtractGlowing
  (params (bIsExtracting :type Boolean))
  (|CallParentFunction bIsExtracting))

(event EventEnterInspector
  (|CallParentFunction))

(event EventExitInspector
  (|CallParentFunction))

(fn ConstructionScript
  (|CallParentFunction)
  (Utilities|FlowControl|Sequence
    (:then_0
      (bind _returnvalue (Rendering|Material|CreateDynamicMaterialInstance (Variables|Default|GetStaticMesh) 0 "/Game/Project/Artist/KeyObj/Material/WineBottle_Glass.WineBottle_Glass" "None" :!class /Script/Engine.PrimitiveComponent))
      (Utilities|Array|Add (Variables|/Game/Project/Core/InteractOBJ/AC_ExtractComponent.AC_ExtractComponent_C|GetExtractMatGroups (Variables|Default|GetAC_ExtractComponent)) _returnvalue))
    (:then_1
      (bind _returnvalue_2 (Rendering|Material|CreateDynamicMaterialInstance (Variables|Default|GetStaticMesh) 1 "/Game/Project/Artist/KeyObj/Material/WineBottle_Cork.WineBottle_Cork" "None" :!class /Script/Engine.PrimitiveComponent))
      (Utilities|Array|Add (Variables|/Game/Project/Core/InteractOBJ/AC_ExtractComponent.AC_ExtractComponent_C|GetExtractMatGroups (Variables|Default|GetAC_ExtractComponent)) _returnvalue_2))))