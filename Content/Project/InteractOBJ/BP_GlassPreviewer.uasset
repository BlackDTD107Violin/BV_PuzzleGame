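; BP_GlassPreviewer is an actor that previews a GLASS totem on a plane through its material.
; On BeginPlay it creates a dynamic instance of M_GlassTotem_Inst on the Plane and stores it.
; ReceiveGLASSPreviewer copies a GLASS's base totem texture and its distance, expand, rotate and scale codes into that material's parameters.
; ClearPreviewer resets those scalar parameters to fixed defaults, leaving the texture as is.
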(event EventBeginPlay
  (bind _returnvalue (Rendering|Material|CreateDynamicMaterialInstance (Variables|Default|GetPlane) 0 "/Game/Project/MaterialLibrary/M_GlassTotem_Inst.M_GlassTotem_Inst" "None" :!class /Script/Engine.PrimitiveComponent))
  (Variables|Default|SetMat_GlassTotem _returnvalue))

(fn ConstructionScript
  (|CallParentFunction))

(fn ClearPreviewer
  (bind _mat_glasstotem (Variables|Default|GetMat_GlassTotem))
  (Rendering|Material|SetScalarParameterValue _mat_glasstotem "Input_Distance" 3.0 :!class /Script/Engine.MaterialInstanceDynamic)
  (Rendering|Material|SetScalarParameterValue _mat_glasstotem "Input_Expand" 0.0 :!class /Script/Engine.MaterialInstanceDynamic)
  (Rendering|Material|SetScalarParameterValue _mat_glasstotem "Input_Rotate" 0.0 :!class /Script/Engine.MaterialInstanceDynamic)
  (Rendering|Material|SetScalarParameterValue _mat_glasstotem "Input_Scaling" 3.0 :!class /Script/Engine.MaterialInstanceDynamic))

(fn ReceiveGLASSPreviewer
  (params (CurrentGLASS :type ST%20Glass%20Collection%20Structure))
  (bind (_targetglassactor _slotcode _itempreview _basetotem _glasstype _code_rotate _code_expand _code_distance _code_scale) (Utilities|Struct|BreakST_GlassCollection CurrentGLASS))
  (bind _mat_glasstotem (Variables|Default|GetMat_GlassTotem))
  (Rendering|Material|SetTextureParameterValue _mat_glasstotem "MainTotem" _basetotem)
  (Rendering|Material|SetScalarParameterValue _mat_glasstotem "Input_Distance" (Math|Conversions|ToFloat(Integer) _code_distance) :!class /Script/Engine.MaterialInstanceDynamic)
  (Rendering|Material|SetScalarParameterValue _mat_glasstotem "Input_Expand" (Math|Conversions|ToFloat(Integer) _code_expand) :!class /Script/Engine.MaterialInstanceDynamic)
  (Rendering|Material|SetScalarParameterValue _mat_glasstotem "Input_Rotate" (Math|Conversions|ToFloat(Integer) _code_rotate) :!class /Script/Engine.MaterialInstanceDynamic)
  (Rendering|Material|SetScalarParameterValue _mat_glasstotem "Input_Scaling" (Math|Conversions|ToFloat(Integer) _code_scale) :!class /Script/Engine.MaterialInstanceDynamic))