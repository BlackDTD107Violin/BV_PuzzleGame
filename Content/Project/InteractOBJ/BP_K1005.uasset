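; BP_K1005 is an interactable object that can be inspected and is removed from the world afterward.
; Entering inspection plays the interact sound, hides the static mesh and calls PickOutOBJ on the CurrentInsertedExtractTA it is inserted in, if valid.
; Exiting inspection replays the sound, then hides the actor and disables its collision.
; BeginPlay runs the parent logic and caches the first-person player character.
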(event EventBeginPlay
  (|CallParentFunction)
  (bind _asbp_first_person_character (Utilities|Casting|CastToBP_FirstPersonCharacter (Game|GetPlayerCharacter 0)))
  (Variables|Default|SetPlayer _asbp_first_person_character))

(event EventEnterInspector
  (Audio|SpawnSoundAttached (Variables|Default|GetInteractSE) (Variables|Default|GetStaticMesh) "None" "0, 0, 0" "0, 0, 0" "KeepRelativeOffset" false 1.0 1.0 0.0 0 0)
  (Development|SetHiddeninGame (Variables|Default|GetStaticMesh) true false)
  (Utilities|IsValid (Variables|Default|GetCurrentInsertedExtractTA)
    (:Is%20Valid
      (Default|PickOutOBJ (Variables|Default|GetCurrentInsertedExtractTA)))))

(event EventExitInspector
  (Audio|SpawnSoundAttached (Variables|Default|GetInteractSE) (Variables|Default|GetStaticMesh) "None" "0, 0, 0" "0, 0, 0" "KeepRelativeOffset" false 1.0 1.0 0.0 0 0)
  (Rendering|SetActorHiddenInGame true)
  (Collision|SetActorEnableCollision false))

(fn ConstructionScript
  (|CallParentFunction))