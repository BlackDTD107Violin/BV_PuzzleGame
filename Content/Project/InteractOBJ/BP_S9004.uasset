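; Clickable rotary handle on the BP_S9002 interact panel that selects a GLASS code unit, draggable only while GLASS is inserted.
; Dragging derives the mouse angle around the handle's projected screen position using 2D dot and cross products.
; Actual mode steps rotation by drag direction with sound, while fast mode follows the angle directly.
; On release it picks a nearby unit angle, updates the panel and eases into place with a lock sound.
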(event OnClicked(SM_Mixer_Turn_Handle)
  (params (TouchedComponent :type Primitive%20Component%20Object%20Reference) (ButtonPressed :type Key%20Structure :default "None"))
  (Variables|Default|SetbIsDragging true)
  (Variables|/Game/ProjectDefault/FirstPerson/Blueprints/BP_FirstPersonCharacter.BP_FirstPersonCharacter_C|SetCurrentInteract (Variables|Default|GetPlayer) self))

(event Custom|SetPivotWhenZoomIn
  (if (not (Variables|Default|GetbHaveSetViewportCenter))
    (Utilities|FlowControl|Delay 0.6)
    (Variables|Default|SetViewportCenter (.ScreenPosition (Class|GameplayStatics|ProjectWorldtoScreen (Game|GetPlayerController 0) (Transformation|GetWorldLocation (Variables|Default|GetSM_Mixer_Turn_Handle)) false)))
    (Variables|Default|SetbHaveSetViewportCenter true)))

(event EventBeginPlay
  (bind _returnvalue (Game|GetPlayerController 0))
  (|CallParentFunction)
  (bind _asbp_first_person_character (Utilities|Casting|CastToBP_FirstPersonCharacter (Game|GetPlayerCharacter 0)))
  (Variables|Default|SetPlayer _asbp_first_person_character)
  (Input|EnableInput _returnvalue)
  (Variables|/Script/Engine.PlayerController|SetbEnableClickEvents _returnvalue true)
  (Variables|/Script/Engine.PlayerController|SetbEnableMouseOverEvents _returnvalue true)
  (bind _asbp_s9002 (Utilities|Casting|CastToBP_S9002 (Actor|GetParentActor)))
  (Variables|Default|SetREF_%20InteractPanel _asbp_s9002))

(event EventTick
  (params (DeltaSeconds :type Float%20%28single-precision%29))
  (CallFunction|CheckState))

(event EventInteractEnd
  (Variables|Default|SetbIsDragging false))

(fn ConstructionScript
  (|CallParentFunction))

(fn BacktoDefault
  (Variables|Default|SetInsertedGLASSUnits 0)
  (Variables|Default|SetbHasInsertedGLASS false)
  (Default|UpdateGLASSCodefromEachFunc (Variables|Default|GetREF_%20InteractPanel))
  (Variables|Default|SetTargetUnitsAngleZ (Utilities|Array|Get(acopy) (Variables|Default|GetUnits) (Variables|Default|GetInsertedGLASSUnits)))
  (Variables|Default|SetbGetTargetUnit true))

(fn CheckNearestUnits
  (bind _output_get (LocalVariables|SetL_CurrentAngleZ (Class|KismetMathLibrary|ClampAxis (.yaw (Variables|/Script/Engine.SceneComponent|GetRelativeRotation (Variables|Default|GetSM_Mixer_Turn_Handle))))))
  (if (>= _output_get 3.3e+02)
    (LocalVariables|SetL_CurrentAngleZ -3e+01))
  (bind (_array_element _array_index) (Utilities|Array|ForEachLoopwithBreak (Variables|Default|GetUnits) :!label _label)
    (:LoopBody
      (Variables|Default|SetTargetUnitsAngleZ _array_element)
      (Variables|Default|SetInsertedGLASSUnits _array_index)
      (if (<= (Math|Float|Absolute(Float) (- (Variables|Default|GetTargetUnitsAngleZ) (LocalVariables|GetL_CurrentAngleZ))) 3e+01)
        (goto _label Break)))))

(fn CheckState
  (if (Variables|Default|GetbHasInsertedGLASS)
    (if (Variables|Default|GetbIsDragging)
      (Variables|Default|SetbGetTargetUnit false)
      (if (Variables|Default|GetbIsActualMode)
        (CallFunction|DragViaInput)
        (CallFunction|RotatebyClockwise)
        (else
          (CallFunction|DragViaInputFastMode)))
      (else
        (if (Variables|Default|GetbGetTargetUnit) :!label _label
          _
          (else
            (CallFunction|CheckNearestUnits)
            (Variables|Default|SetbGetTargetUnit true)
            (Default|UpdateGLASSCodefromEachFunc (Variables|Default|GetREF_%20InteractPanel))))
        (CallFunction|GotoTargetUnit)))
    (else
      (goto _label))))

(fn DragViaInput
  (Utilities|FlowControl|Sequence
    (:then_0
      (bind (_dotvalue _bcrossresult) (CallFunction|UpdateTriggerMousePivot))
      (LocalVariables|SetLCurrentDotVal _dotvalue)
      (bind _output_get (LocalVariables|SetL_CurrentIsRightSide _bcrossresult))
      (if _output_get
        (LocalVariables|SetL_CurrentAngle (Class|KismetMathLibrary|DegAcos (LocalVariables|GetLCurrentDotVal)))
        (else
          (LocalVariables|SetL_CurrentAngle (- 3.6e+02 (Class|KismetMathLibrary|DegAcos (LocalVariables|GetLCurrentDotVal)))))))
    (:then_1
      (if (== (LocalVariables|GetL_CurrentIsRightSide) (Variables|Default|GetbIsRightSide))
        (bind _output_get_2 (Variables|Default|SetbHasUpdateMousePivot (!= 0.0 (- (LocalVariables|GetL_CurrentAngle) (Variables|Default|GetLatestAngle))) :!label _label))
        (if _output_get_2
          (Variables|Default|SetbIsClockwise (> (- (LocalVariables|GetL_CurrentAngle) (Variables|Default|GetLatestAngle)) 0.0))
          (Variables|Default|SetLatestAngle (LocalVariables|GetL_CurrentAngle) :!label _label_2)
          (Variables|Default|SetLatestDotVal (LocalVariables|GetLCurrentDotVal))
          (Variables|Default|SetbIsRightSide (LocalVariables|GetL_CurrentIsRightSide))
          (Variables|Default|SetbMeshReachLimit false))
        (elif (< (LocalVariables|GetLCurrentDotVal) 0.0)
          (goto _label)
          (else
            (Variables|Default|SetbIsClockwise (LocalVariables|GetL_CurrentIsRightSide))
            (goto _label_2)))))))

(fn DragViaInputFastMode
  (bind _sm_mixer_turn_handle (Variables|Default|GetSM_Mixer_Turn_Handle))
  (bind _sm_mixer_turn_handle_2 (Variables|Default|GetSM_Mixer_Turn_Handle))
  (bind _relativerotation (Variables|/Script/Engine.SceneComponent|GetRelativeRotation _sm_mixer_turn_handle))
  (bind _relativerotation_2 (Variables|/Script/Engine.SceneComponent|GetRelativeRotation _sm_mixer_turn_handle_2))
  (bind (_dotvalue _bcrossresult _acosdvalue) (CallFunction|UpdateTriggerMousePivot))
  (if _bcrossresult
    (Transformation|SetRelativeRotation _sm_mixer_turn_handle (Math|Rotator|MakeRotator (.roll _relativerotation) (.pitch _relativerotation) _acosdvalue) false false)
    (else
      (Transformation|SetRelativeRotation _sm_mixer_turn_handle_2 (Math|Rotator|MakeRotator (.roll _relativerotation_2) (.pitch _relativerotation_2) (- 3.6e+02 _acosdvalue)) false false))))

(fn GotoTargetUnit
  (bind _targetunitsanglez (Variables|Default|GetTargetUnitsAngleZ))
  (bind _sm_mixer_turn_handle (Variables|Default|GetSM_Mixer_Turn_Handle))
  (bind _sm_mixer_turn_handle_2 (Variables|Default|GetSM_Mixer_Turn_Handle))
  (bind _sm_mixer_turn_handle_3 (Variables|Default|GetSM_Mixer_Turn_Handle))
  (bind _relativerotation (Variables|/Script/Engine.SceneComponent|GetRelativeRotation _sm_mixer_turn_handle_3))
  (bind _relativerotation_2 (Variables|/Script/Engine.SceneComponent|GetRelativeRotation _sm_mixer_turn_handle))
  (bind _relativerotation_3 (Variables|/Script/Engine.SceneComponent|GetRelativeRotation _sm_mixer_turn_handle_2))
  (bind _returnvalue (- (.yaw _relativerotation) _targetunitsanglez))
  (bind _returnvalue_2 (Math|Float|Absolute(Float) _returnvalue))
  (Utilities|FlowControl|Sequence
    (:then_0
      (Transformation|SetRelativeRotation (Variables|Default|GetSM_Mixer_Turn_Handle) (Math|Interpolation|RInterpTo (Variables|/Script/Engine.SceneComponent|GetRelativeRotation _sm_mixer_turn_handle_2) (Math|Rotator|MakeRotator (.roll _relativerotation_3) (.pitch _relativerotation_3) (Variables|Default|GetTargetUnitsAngleZ)) (Utilities|Time|GetWorldDeltaSeconds) 4.0) false false))
    (:then_1
      (if (or (<= _returnvalue_2 0.2) (<= (Math|Float|Absolute(Float) (- _returnvalue_2 3.6e+02)) 0.2))
        (Transformation|SetRelativeRotation _sm_mixer_turn_handle (Math|Rotator|MakeRotator (.roll _relativerotation_2) (.pitch _relativerotation_2) (Variables|Default|GetTargetUnitsAngleZ)) false false)
        (if (not (Variables|Default|GetbMeshReachLimit))
          (Variables|Default|SetbMeshReachLimit true)
          (Audio|SpawnSoundAttached "/Game/Project/Audio/MetaSoundSource/SE/MSS_MetalLock_4.MSS_MetalLock_4" (Variables|Default|GetSM_Mixer_Turn_Handle) "None" "0, 0, 0" "0, 0, 0" "KeepRelativeOffset" false 1.0 1.0 0.0 0 0)
          (Variables|Default|SetbSoundPlaying false))))))

(fn ReceiveGLASScode
  (params (Code :type Integer))
  (Variables|Default|SetInsertedGLASSUnits Code)
  (Variables|Default|SetbHasInsertedGLASS true)
  (Default|UpdateGLASSCodefromEachFunc (Variables|Default|GetREF_%20InteractPanel))
  (Variables|Default|SetTargetUnitsAngleZ (Utilities|Array|Get(acopy) (Variables|Default|GetUnits) (Variables|Default|GetInsertedGLASSUnits)))
  (Variables|Default|SetbGetTargetUnit true))

(fn RotatebyClockwise
  (if (Variables|Default|GetbHasUpdateMousePivot)
    (Utilities|FlowControl|Sequence
      (:then_0
        (if (Variables|Default|GetbIsClockwise)
          (Transformation|AddLocalRotation (Variables|Default|GetSM_Mixer_Turn_Handle) (Math|Rotator|MakeRotator 0.0 0.0 (Variables|Default|GetDefaultSpeed)) false false)
          (else
            (Transformation|AddLocalRotation (Variables|Default|GetSM_Mixer_Turn_Handle) (Math|Rotator|MakeRotator 0.0 0.0 (* (Variables|Default|GetDefaultSpeed) -1.0)) false false))))
      (:then_1
        (if (or (not (Utilities|IsValid (Variables|Default|GetAudioEnable_Handle))) (not (Variables|Default|GetbSoundPlaying)))
          (Variables|Default|SetbSoundPlaying true)
          (bind _returnvalue (Audio|SpawnSoundAttached "/Game/Project/Audio/MetaSoundSource/SE/MSS_ScaleSlider_8.MSS_ScaleSlider_8" (Variables|Default|GetSM_Mixer_Turn_Handle) "None" "0, 0, 0" "0, 0, 0" "KeepRelativeOffset" false 1.0 1.0 0.0 0 0))
          (Variables|Default|SetAudioEnable_Handle _returnvalue))))))

(fn UpdateTriggerMousePivot
  (bind _returnvalue (Math|Vector2D|MakeVector2D 0.0 -1.0))
  (bind _returnvalue_2 (Game|GetPlayerController 0))
  (bind _viewportcenter (Variables|Default|GetViewportCenter))
  (bind _worldlocation (Game|Player|ConvertMouseLocationToWorldSpace _returnvalue_2))
  (bind _screenlocation (Class|PlayerController|ProjectWorldLocationtoScreen _returnvalue_2 _worldlocation false))
  (bind _returnvalue_3 (- _screenlocation _viewportcenter))
  (bind _returnvalue_4 (Math|Vector2D|Normalize2D _returnvalue_3))
  (bind _returnvalue_5 (Math|Vector2D|DotProduct(2D) _returnvalue_4 _returnvalue))
  (return _returnvalue_5 (< (Class|KismetMathLibrary|CrossProduct2D _returnvalue_4 _returnvalue) 0.0) (Class|KismetMathLibrary|DegAcos _returnvalue_5)))