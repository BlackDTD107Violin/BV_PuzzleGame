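; BP_S1101 is an interactable box with a camera zoom view, where the player mouse-drags the lock open, then the cover.
; Zooming blends the view to the box, blocks move/look input and swaps trigger and part collision.
; Tick turns vertical mouse movement into rotation steps, mirrored on pivot components and Anim Blueprint variables, with slide and finish sounds.
; Parts released past a threshold angle interpolate to their end pose.
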(event OnClicked(Cover)
  (params (TouchedComponent :type Primitive%20Component%20Object%20Reference) (ButtonPressed :type Key%20Structure :default "None"))
  (if (and (not (Variables|Default|GetbCoverIsFinish)) (Variables|Default|GetbLockIsFinish))
    (Variables|Default|SetbIsDraggingCover true)
    (Variables|/Game/ProjectDefault/FirstPerson/Blueprints/BP_FirstPersonCharacter.BP_FirstPersonCharacter_C|SetCurrentInteract (Variables|Default|GetPlayer) self)))

(event OnClicked(Lock)
  (params (TouchedComponent :type Primitive%20Component%20Object%20Reference) (ButtonPressed :type Key%20Structure :default "None"))
  (if (not (Variables|Default|GetbLockIsFinish))
    (Variables|Default|SetbIsDraggingLock true)
    (Variables|/Game/ProjectDefault/FirstPerson/Blueprints/BP_FirstPersonCharacter.BP_FirstPersonCharacter_C|SetCurrentInteract (Variables|Default|GetPlayer) self)))

(event EventBeginPlay
  (bind _returnvalue (Game|GetPlayerController 0))
  (|CallParentFunction)
  (bind _asbp_first_person_character (Utilities|Casting|CastToBP_FirstPersonCharacter (Game|GetPlayerCharacter 0)))
  (Variables|Default|SetPlayer _asbp_first_person_character)
  (Input|EnableInput _returnvalue)
  (Variables|/Script/Engine.PlayerController|SetbEnableClickEvents _returnvalue true)
  (Variables|/Script/Engine.PlayerController|SetbEnableMouseOverEvents _returnvalue true)
  (CallFunction|AssignZoominGroup)
  (bind _assk_learning_box_01_skeleton_anim_blueprint (Utilities|Casting|CastToSK_LearningBox_01_Skeleton_AnimBlueprint (Components|SkeletalMesh|GetAnimInstance (Variables|Default|GetSK_LearningBox_01))))
  (Variables|Default|SetREF_ThisAnimGraph _assk_learning_box_01_skeleton_anim_blueprint))

(event EventZoomin
  (params (ZoomComponent :type Actor%20Component%20Object%20Reference))
  (bind _returnvalue (Game|GetPlayerController 0))
  (Game|Player|SetViewTargetwithBlend (Game|GetPlayerController 0) self 0.5 "VTBlend_Linear" 0.0 true)
  (Input|SetIgnoreMoveInput _returnvalue true)
  (Input|SetIgnoreLookInput _returnvalue true)
  (Default|ClearGamePromptUIView (Variables|Default|GetPlayer))
  (Collision|SetCollisionProfileName (Variables|Default|GetZoom%20Trigger_Main) "NoCollision" true :!class /Script/Engine.PrimitiveComponent)
  (for _array_element (Variables|Default|GetMeshGroup)
    (Collision|SetCollisionProfileName _array_element "BlockAllDynamic" true :!class /Script/Engine.PrimitiveComponent)))

(event EventTick
  (params (DeltaSeconds :type Float%20%28single-precision%29))
  (if (Variables|Default|GetbLockIsFinish)
    (if (not (Variables|Default|GetbCoverIsFinish))
      (CallFunction|CheckCoverState))
    (else
      (CallFunction|CheckLockState))))

(event EventZoomOut
  (bind _returnvalue (Game|GetPlayerController 0))
  (Game|Player|SetViewTargetwithBlend (Game|GetPlayerController 0) (Game|GetPlayerCharacter 0) 0.5 "VTBlend_Linear" 0.0 true)
  (Input|ResetIgnoreMoveInput _returnvalue)
  (Input|ResetIgnoreLookInput _returnvalue)
  (Utilities|FlowControl|Delay 0.5)
  (Collision|SetCollisionProfileName (Variables|Default|GetZoom%20Trigger_Main) "BlockAllDynamic" true :!class /Script/Engine.PrimitiveComponent)
  (for _array_element (Variables|Default|GetMeshGroup)
    (Collision|SetCollisionProfileName _array_element "NoCollision" true :!class /Script/Engine.PrimitiveComponent)))

(event EventInteractEnd
  (CallFunction|CancelingDrag)
  (Variables|/Game/ProjectDefault/FirstPerson/Blueprints/BP_FirstPersonCharacter.BP_FirstPersonCharacter_C|SetCurrentInteract (Variables|Default|GetPlayer) self)
  (Variables|Default|SetbSoundPlaying false))

(event EventInteract
  (params (InteractActor :type Actor%20Object%20Reference) (InteractTarget :type Actor%20Component%20Object%20Reference))
  (CallFunction|Zoomin InteractTarget))

(fn ConstructionScript
  (|CallParentFunction))

(fn UpdateTriggerMousePivot
  (bind _returnvalue (Game|GetPlayerController 0))
  (Variables|Default|SetTriggerMousePivot (.ScreenLocation (Class|PlayerController|ProjectWorldLocationtoScreen _returnvalue (.WorldLocation (Game|Player|ConvertMouseLocationToWorldSpace _returnvalue)) false))))

(fn DragLockViaInput
  (bind _returnvalue (Game|GetPlayerController 0))
  (bind _triggermousepivot (Variables|Default|GetTriggerMousePivot))
  (bind _ref_thisanimgraph (Variables|Default|GetREF_ThisAnimGraph))
  (bind _ref_thisanimgraph_2 (Variables|Default|GetREF_ThisAnimGraph))
  (bind _worldlocation (Game|Player|ConvertMouseLocationToWorldSpace _returnvalue))
  (bind _screenlocation (Class|PlayerController|ProjectWorldLocationtoScreen _returnvalue _worldlocation false))
  (if (not (Variables|Default|GetbLockIsFinish))
    (if (!= (.y _screenlocation) (.y _triggermousepivot))
      (if (> (.y _screenlocation) (.y _triggermousepivot))
        (Transformation|AddLocalRotation (Variables|Default|GetLockPivot) (Math|Rotator|MakeRotator (Variables|Default|GetRotateSpeed) 0.0 0.0) false false)
        (bind _output_get (Variables|/Game/Project/Artist/Gadget/Mesh/SK_LearningBox_01_Skeleton_AnimBlueprint.SK_LearningBox_01_Skeleton_AnimBlueprint_C|SetLock%20Rotation _ref_thisanimgraph_2 (Math|Rotator|MakeRotator (+ (Variables|Default|GetRotateSpeed) (.roll (Variables|/Game/Project/Artist/Gadget/Mesh/SK_LearningBox_01_Skeleton_AnimBlueprint.SK_LearningBox_01_Skeleton_AnimBlueprint_C|GetLock%20Rotation _ref_thisanimgraph_2))) (.pitch (Variables|/Game/Project/Artist/Gadget/Mesh/SK_LearningBox_01_Skeleton_AnimBlueprint.SK_LearningBox_01_Skeleton_AnimBlueprint_C|GetLock%20Rotation _ref_thisanimgraph_2)) (.yaw (Variables|/Game/Project/Artist/Gadget/Mesh/SK_LearningBox_01_Skeleton_AnimBlueprint.SK_LearningBox_01_Skeleton_AnimBlueprint_C|GetLock%20Rotation _ref_thisanimgraph_2)))))
        (if (>= (.roll _output_get) 0.0)
          (Variables|/Game/Project/Artist/Gadget/Mesh/SK_LearningBox_01_Skeleton_AnimBlueprint.SK_LearningBox_01_Skeleton_AnimBlueprint_C|SetLock%20Rotation (Variables|Default|GetREF_ThisAnimGraph) "0, 0, 0")
          (Transformation|SetRelativeRotation (Variables|Default|GetLockPivot) "0, 0, 0" false false)
          (else
            (CallFunction|UpdateTriggerMousePivot)
            (if (not (Variables|Default|GetbSoundPlaying))
              (Variables|Default|SetbSoundPlaying true)
              (Audio|SpawnSoundAttached "/Game/Project/Audio/MetaSoundSource/MSS_S0003_LockSlide.MSS_S0003_LockSlide" (Variables|Default|GetSK_LearningBox_01) "None" "0, 0, 0" "0, 0, 0" "KeepRelativeOffset" false 1.0 1.0 0.0 0 0))))
        (else
          (Transformation|AddLocalRotation (Variables|Default|GetLockPivot) (Math|Rotator|MakeRotator (* (Variables|Default|GetRotateSpeed) -1.0) 0.0 0.0) false false)
          (bind _output_get_2 (Variables|/Game/Project/Artist/Gadget/Mesh/SK_LearningBox_01_Skeleton_AnimBlueprint.SK_LearningBox_01_Skeleton_AnimBlueprint_C|SetLock%20Rotation _ref_thisanimgraph (Math|Rotator|MakeRotator (+ (* (Variables|Default|GetRotateSpeed) -1.0) (.roll (Variables|/Game/Project/Artist/Gadget/Mesh/SK_LearningBox_01_Skeleton_AnimBlueprint.SK_LearningBox_01_Skeleton_AnimBlueprint_C|GetLock%20Rotation _ref_thisanimgraph))) (.pitch (Variables|/Game/Project/Artist/Gadget/Mesh/SK_LearningBox_01_Skeleton_AnimBlueprint.SK_LearningBox_01_Skeleton_AnimBlueprint_C|GetLock%20Rotation _ref_thisanimgraph)) (.yaw (Variables|/Game/Project/Artist/Gadget/Mesh/SK_LearningBox_01_Skeleton_AnimBlueprint.SK_LearningBox_01_Skeleton_AnimBlueprint_C|GetLock%20Rotation _ref_thisanimgraph)))))
          (if (<= (Class|KismetMathLibrary|ClampAxis (.roll _output_get_2)) 1.8e+02)
            (Variables|Default|SetbLockIsFinish true)
            (CallFunction|CancelingDrag)
            (Audio|SpawnSoundAttached "/Game/Project/Audio/MetaSoundSource/MSS_S0003_LockFinish.MSS_S0003_LockFinish" (Variables|Default|GetSK_LearningBox_01) "None" "0, 0, 0" "0, 0, 0" "KeepRelativeOffset" false 1.0 1.0 0.0 0 0)
            (Variables|Default|SetbSoundPlaying false)
            (else
              (CallFunction|UpdateTriggerMousePivot)
              (if (not (Variables|Default|GetbSoundPlaying))
                (Variables|Default|SetbSoundPlaying true)
                (Audio|SpawnSoundAttached "/Game/Project/Audio/MetaSoundSource/MSS_S0003_LockSlide.MSS_S0003_LockSlide" (Variables|Default|GetSK_LearningBox_01) "None" "0, 0, 0" "0, 0, 0" "KeepRelativeOffset" false 1.0 1.0 0.0 0 0)))))))))

(fn DragCoverViaInput
  (bind _returnvalue (Game|GetPlayerController 0))
  (bind _triggermousepivot (Variables|Default|GetTriggerMousePivot))
  (bind _ref_thisanimgraph (Variables|Default|GetREF_ThisAnimGraph))
  (bind _ref_thisanimgraph_2 (Variables|Default|GetREF_ThisAnimGraph))
  (bind _worldlocation (Game|Player|ConvertMouseLocationToWorldSpace _returnvalue))
  (bind _screenlocation (Class|PlayerController|ProjectWorldLocationtoScreen _returnvalue _worldlocation false))
  (if (not (Variables|Default|GetbCoverIsFinish))
    (if (!= (.y _screenlocation) (.y _triggermousepivot))
      (if (> (.y _screenlocation) (.y _triggermousepivot))
        (Transformation|AddLocalRotation (Variables|Default|GetCoverPivot) (Math|Rotator|MakeRotator (Variables|Default|GetRotateSpeed) 0.0 0.0) false false)
        (bind _output_get (Variables|/Game/Project/Artist/Gadget/Mesh/SK_LearningBox_01_Skeleton_AnimBlueprint.SK_LearningBox_01_Skeleton_AnimBlueprint_C|SetCoverRotation _ref_thisanimgraph (Math|Rotator|MakeRotator (+ (Variables|Default|GetRotateSpeed) (.roll (Variables|/Game/Project/Artist/Gadget/Mesh/SK_LearningBox_01_Skeleton_AnimBlueprint.SK_LearningBox_01_Skeleton_AnimBlueprint_C|GetCoverRotation _ref_thisanimgraph))) (.pitch (Variables|/Game/Project/Artist/Gadget/Mesh/SK_LearningBox_01_Skeleton_AnimBlueprint.SK_LearningBox_01_Skeleton_AnimBlueprint_C|GetCoverRotation _ref_thisanimgraph)) (.yaw (Variables|/Game/Project/Artist/Gadget/Mesh/SK_LearningBox_01_Skeleton_AnimBlueprint.SK_LearningBox_01_Skeleton_AnimBlueprint_C|GetCoverRotation _ref_thisanimgraph)))))
        (if (>= (.roll _output_get) 0.0)
          (Variables|/Game/Project/Artist/Gadget/Mesh/SK_LearningBox_01_Skeleton_AnimBlueprint.SK_LearningBox_01_Skeleton_AnimBlueprint_C|SetCoverRotation (Variables|Default|GetREF_ThisAnimGraph) "0.0,0.0,0.0")
          (Transformation|SetRelativeRotation (Variables|Default|GetCoverPivot) "0, 0, 0" false false)
          (else
            (CallFunction|UpdateTriggerMousePivot)
            (if (not (Variables|Default|GetbSoundPlaying))
              (Variables|Default|SetbSoundPlaying true)
              (Audio|SpawnSoundAttached "/Game/Project/Audio/MetaSoundSource/MSS_S0003_CoverSlide.MSS_S0003_CoverSlide" (Variables|Default|GetSK_LearningBox_01) "None" "0, 0, 0" "0, 0, 0" "KeepRelativeOffset" false 1.0 1.0 0.0 0 0))))
        (else
          (Transformation|AddLocalRotation (Variables|Default|GetCoverPivot) (Math|Rotator|MakeRotator (* (Variables|Default|GetRotateSpeed) -1.0) 0.0 0.0) false false)
          (bind _output_get_2 (Variables|/Game/Project/Artist/Gadget/Mesh/SK_LearningBox_01_Skeleton_AnimBlueprint.SK_LearningBox_01_Skeleton_AnimBlueprint_C|SetCoverRotation _ref_thisanimgraph_2 (Math|Rotator|MakeRotator (+ (* (Variables|Default|GetRotateSpeed) -1.0) (.roll (Variables|/Game/Project/Artist/Gadget/Mesh/SK_LearningBox_01_Skeleton_AnimBlueprint.SK_LearningBox_01_Skeleton_AnimBlueprint_C|GetCoverRotation _ref_thisanimgraph_2))) (.pitch (Variables|/Game/Project/Artist/Gadget/Mesh/SK_LearningBox_01_Skeleton_AnimBlueprint.SK_LearningBox_01_Skeleton_AnimBlueprint_C|GetCoverRotation _ref_thisanimgraph_2)) (.yaw (Variables|/Game/Project/Artist/Gadget/Mesh/SK_LearningBox_01_Skeleton_AnimBlueprint.SK_LearningBox_01_Skeleton_AnimBlueprint_C|GetCoverRotation _ref_thisanimgraph_2)))))
          (if (<= (Class|KismetMathLibrary|ClampAxis (.roll _output_get_2)) 2.7e+02)
            (Variables|Default|SetbCoverIsFinish true)
            (CallFunction|CancelingDrag)
            (Collision|SetCollisionProfileName (Variables|Default|GetStaticMesh) "TRICKignore" true :!class /Script/Engine.PrimitiveComponent)
            (Audio|SpawnSoundAttached "/Game/Project/Audio/MetaSoundSource/MSS_S0003_CoverFinish.MSS_S0003_CoverFinish" (Variables|Default|GetSK_LearningBox_01) "None" "0, 0, 0" "0, 0, 0" "KeepRelativeOffset" false 1.0 1.0 0.0 0 0)
            (Variables|Default|SetbSoundPlaying false)
            (else
              (CallFunction|UpdateTriggerMousePivot)
              (if (not (Variables|Default|GetbSoundPlaying))
                (Variables|Default|SetbSoundPlaying true)
                (Audio|SpawnSoundAttached "/Game/Project/Audio/MetaSoundSource/MSS_S0003_CoverSlide.MSS_S0003_CoverSlide" (Variables|Default|GetSK_LearningBox_01) "None" "0, 0, 0" "0, 0, 0" "KeepRelativeOffset" false 1.0 1.0 0.0 0 0)))))))))

(fn CancelingDrag
  (Variables|Default|SetbIsDraggingLock false)
  (Variables|Default|SetbIsDraggingCover false)
  (Variables|Default|SetbHasUpdateMousePivot false))

(fn FinishRemainingAngleLock
  (bind _lockpivot (Variables|Default|GetLockPivot))
  (bind _ref_thisanimgraph (Variables|Default|GetREF_ThisAnimGraph))
  (bind _lockpivot_2 (Variables|Default|GetLockPivot))
  (bind _relativerotation (Variables|/Script/Engine.SceneComponent|GetRelativeRotation _lockpivot))
  (bind _relativerotation_2 (Variables|/Script/Engine.SceneComponent|GetRelativeRotation _lockpivot_2))
  (Utilities|FlowControl|Sequence
    (:then_0
      (Variables|/Game/Project/Artist/Gadget/Mesh/SK_LearningBox_01_Skeleton_AnimBlueprint.SK_LearningBox_01_Skeleton_AnimBlueprint_C|SetLock%20Rotation (Variables|Default|GetREF_ThisAnimGraph) (Math|Interpolation|RInterpTo (Variables|/Game/Project/Artist/Gadget/Mesh/SK_LearningBox_01_Skeleton_AnimBlueprint.SK_LearningBox_01_Skeleton_AnimBlueprint_C|GetLock%20Rotation _ref_thisanimgraph) (Math|Rotator|MakeRotator -1.8e+02 (.pitch (Variables|/Game/Project/Artist/Gadget/Mesh/SK_LearningBox_01_Skeleton_AnimBlueprint.SK_LearningBox_01_Skeleton_AnimBlueprint_C|GetLock%20Rotation _ref_thisanimgraph)) (.yaw (Variables|/Game/Project/Artist/Gadget/Mesh/SK_LearningBox_01_Skeleton_AnimBlueprint.SK_LearningBox_01_Skeleton_AnimBlueprint_C|GetLock%20Rotation _ref_thisanimgraph))) (Utilities|Time|GetWorldDeltaSeconds) 4.0))
      (Transformation|SetRelativeRotation (Variables|Default|GetLockPivot) (Math|Interpolation|RInterpTo (Variables|/Script/Engine.SceneComponent|GetRelativeRotation (Variables|Default|GetLockPivot)) (Math|Rotator|MakeRotator -1.8e+02 (.pitch _relativerotation) (.yaw _relativerotation)) (Utilities|Time|GetWorldDeltaSeconds) 4.0) false false))
    (:then_1
      (if (<= (.roll (Variables|/Game/Project/Artist/Gadget/Mesh/SK_LearningBox_01_Skeleton_AnimBlueprint.SK_LearningBox_01_Skeleton_AnimBlueprint_C|GetLock%20Rotation (Variables|Default|GetREF_ThisAnimGraph))) -179.0)
        (Variables|/Game/Project/Artist/Gadget/Mesh/SK_LearningBox_01_Skeleton_AnimBlueprint.SK_LearningBox_01_Skeleton_AnimBlueprint_C|SetLock%20Rotation (Variables|Default|GetREF_ThisAnimGraph) "0.000000,0.000000,-180.000000")
        (Transformation|SetRelativeRotation (Variables|Default|GetLockPivot) (Math|Rotator|MakeRotator -1.8e+02 (.pitch _relativerotation_2) (.yaw _relativerotation_2)) false false)
        (Variables|Default|SetbLockIsFinish true)
        (CallFunction|CancelingDrag)
        (Audio|SpawnSoundAttached "/Game/Project/Audio/MetaSoundSource/MSS_S0003_LockFinish.MSS_S0003_LockFinish" (Variables|Default|GetSK_LearningBox_01) "None" "0, 0, 0" "0, 0, 0" "KeepRelativeOffset" false 1.0 1.0 0.0 0 0)
        (Variables|Default|SetbSoundPlaying false)))))

(fn FinishRemainingAngleCover
  (bind _coverpivot (Variables|Default|GetCoverPivot))
  (bind _ref_thisanimgraph (Variables|Default|GetREF_ThisAnimGraph))
  (bind _coverpivot_2 (Variables|Default|GetCoverPivot))
  (bind _relativerotation (Variables|/Script/Engine.SceneComponent|GetRelativeRotation _coverpivot_2))
  (bind _relativerotation_2 (Variables|/Script/Engine.SceneComponent|GetRelativeRotation _coverpivot))
  (Utilities|FlowControl|Sequence
    (:then_0
      (Variables|/Game/Project/Artist/Gadget/Mesh/SK_LearningBox_01_Skeleton_AnimBlueprint.SK_LearningBox_01_Skeleton_AnimBlueprint_C|SetCoverRotation (Variables|Default|GetREF_ThisAnimGraph) (Math|Interpolation|RInterpTo (Variables|/Game/Project/Artist/Gadget/Mesh/SK_LearningBox_01_Skeleton_AnimBlueprint.SK_LearningBox_01_Skeleton_AnimBlueprint_C|GetCoverRotation _ref_thisanimgraph) (Math|Rotator|MakeRotator -9e+01 (.pitch (Variables|/Game/Project/Artist/Gadget/Mesh/SK_LearningBox_01_Skeleton_AnimBlueprint.SK_LearningBox_01_Skeleton_AnimBlueprint_C|GetCoverRotation _ref_thisanimgraph)) (.yaw (Variables|/Game/Project/Artist/Gadget/Mesh/SK_LearningBox_01_Skeleton_AnimBlueprint.SK_LearningBox_01_Skeleton_AnimBlueprint_C|GetCoverRotation _ref_thisanimgraph))) (Utilities|Time|GetWorldDeltaSeconds) 4.0))
      (Transformation|SetRelativeRotation (Variables|Default|GetCoverPivot) (Math|Interpolation|RInterpTo (Variables|/Script/Engine.SceneComponent|GetRelativeRotation (Variables|Default|GetCoverPivot)) (Math|Rotator|MakeRotator -9e+01 (.pitch _relativerotation) (.yaw _relativerotation)) (Utilities|Time|GetWorldDeltaSeconds) 4.0) false false))
    (:then_1
      (if (<= (.roll (Variables|/Game/Project/Artist/Gadget/Mesh/SK_LearningBox_01_Skeleton_AnimBlueprint.SK_LearningBox_01_Skeleton_AnimBlueprint_C|GetCoverRotation (Variables|Default|GetREF_ThisAnimGraph))) -89.0)
        (Variables|/Game/Project/Artist/Gadget/Mesh/SK_LearningBox_01_Skeleton_AnimBlueprint.SK_LearningBox_01_Skeleton_AnimBlueprint_C|SetLock%20Rotation (Variables|Default|GetREF_ThisAnimGraph) "0.000000,0.000000,-90.000000")
        (Transformation|SetRelativeRotation (Variables|Default|GetCoverPivot) (Math|Rotator|MakeRotator -9e+01 (.pitch _relativerotation_2) (.yaw _relativerotation_2)) false false)
        (Variables|Default|SetbCoverIsFinish true)
        (CallFunction|CancelingDrag)
        (Collision|SetCollisionProfileName (Variables|Default|GetStaticMesh) "TRICKignore" true :!class /Script/Engine.PrimitiveComponent)
        (Audio|SpawnSoundAttached "/Game/Project/Audio/MetaSoundSource/MSS_S0003_CoverFinish.MSS_S0003_CoverFinish" (Variables|Default|GetSK_LearningBox_01) "None" "0, 0, 0" "0, 0, 0" "KeepRelativeOffset" false 1.0 1.0 0.0 0 0)
        (Variables|Default|SetbSoundPlaying false)))))

(fn CheckCoverState
  (if (Variables|Default|GetbIsDraggingCover)
    (if (Variables|Default|GetbHasUpdateMousePivot)
      (CallFunction|DragCoverViaInput)
      (else
        (Variables|Default|SetbHasUpdateMousePivot true)
        (CallFunction|UpdateTriggerMousePivot)))
    (elif (<= (.roll (Variables|/Game/Project/Artist/Gadget/Mesh/SK_LearningBox_01_Skeleton_AnimBlueprint.SK_LearningBox_01_Skeleton_AnimBlueprint_C|GetCoverRotation (Variables|Default|GetREF_ThisAnimGraph))) -6e+01)
      (CallFunction|FinishRemainingAngleCover))))

(fn CheckLockState
  (if (Variables|Default|GetbIsDraggingLock)
    (if (Variables|Default|GetbHasUpdateMousePivot)
      (CallFunction|DragLockViaInput)
      (else
        (Variables|Default|SetbHasUpdateMousePivot true)
        (CallFunction|UpdateTriggerMousePivot)))
    (elif (<= (.roll (Variables|/Game/Project/Artist/Gadget/Mesh/SK_LearningBox_01_Skeleton_AnimBlueprint.SK_LearningBox_01_Skeleton_AnimBlueprint_C|GetLock%20Rotation (Variables|Default|GetREF_ThisAnimGraph))) -9e+01)
      (CallFunction|FinishRemainingAngleLock))))

(fn AssignZoominGroup
  (Utilities|Array|Add (Variables|Default|GetMeshGroup) (Variables|Default|GetCover))
  (Utilities|Array|Add (Variables|Default|GetMeshGroup) (Variables|Default|GetLock)))