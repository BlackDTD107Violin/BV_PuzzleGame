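; Interactable mixer slider handle, a child actor of the BP_S9002 panel, draggable only while a GLASS code is inserted.
; Each tick, vertical mouse movement steps the handle along local X between two limits, with slide and lock sounds.
; When not dragged, it eases to a nearby Units notch and has the panel update its GLASS code.
; Received codes preset the notch; BackToDefault restores the default and locks dragging.
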(event OnClicked(SM_Mixer_Move_Handle)
  (params (TouchedComponent :type Primitive%20Component%20Object%20Reference) (ButtonPressed :type Key%20Structure :default "None"))
  (Variables|Default|SetbIsDragging true)
  (Variables|/Game/ProjectDefault/FirstPerson/Blueprints/BP_FirstPersonCharacter.BP_FirstPersonCharacter_C|SetCurrentInteract (Variables|Default|GetPlayer) self))

(event EventBeginPlay
  (bind _returnvalue (Game|GetPlayerController 0))
  (|CallParentFunction)
  (bind _asbp_first_person_character (Utilities|Casting|CastToBP_FirstPersonCharacter (Game|GetPlayerCharacter 0)))
  (Variables|Default|SetPlayer _asbp_first_person_character)
  (Input|EnableInput _returnvalue)
  (Variables|/Script/Engine.PlayerController|SetbEnableClickEvents _returnvalue true)
  (Variables|/Script/Engine.PlayerController|SetbEnableMouseOverEvents _returnvalue true)
  (bind _asbp_s9002 (Utilities|Casting|CastToBP_S9002 (Actor|GetParentActor)))
  (Variables|Default|SetREF_%20InteractPanel _asbp_s9002))

(event EventTick
  (params (DeltaSeconds :type Float%20%28single-precision%29))
  (CallFunction|CheckState))

(event EventInteractEnd
  (Variables|Default|SetbIsDragging false))

(fn ConstructionScript
  (|CallParentFunction))

(fn BacktoDefault
  (Variables|Default|SetInsertedGLASSUnits 3)
  (Variables|Default|SetbHasInsertedGLASS false)
  (Default|UpdateGLASSCodefromEachFunc (Variables|Default|GetREF_%20InteractPanel))
  (Variables|Default|SetTargetUnitsPosX (Utilities|Array|Get(acopy) (Variables|Default|GetUnits) (Variables|Default|GetInsertedGLASSUnits)))
  (Variables|Default|SetbGetTargetUnit true))

(fn CheckNearestUnits
  (LocalVariables|SetL_CurrentPosX (.x (Variables|/Script/Engine.SceneComponent|GetRelativeLocation (Variables|Default|GetSM_Mixer_Move_Handle))))
  (bind (_array_element _array_index) (Utilities|Array|ForEachLoopwithBreak (Variables|Default|GetUnits) :!label _label)
    (:LoopBody
      (Variables|Default|SetTargetUnitsPosX _array_element)
      (Variables|Default|SetInsertedGLASSUnits _array_index)
      (if (<= (Math|Float|Absolute(Float) (- (Variables|Default|GetTargetUnitsPosX) (LocalVariables|GetL_CurrentPosX))) 6.4)
        (goto _label Break)))))

(fn CheckState
  (if (Variables|Default|GetbHasInsertedGLASS)
    (if (Variables|Default|GetbIsDragging)
      (if (Variables|Default|GetbHasUpdateMousePivot)
        (CallFunction|DragViaInput)
        (else
          (Variables|Default|SetbHasUpdateMousePivot true)
          (CallFunction|UpdateTriggerMousePivot)))
      (else
        (if (Variables|Default|GetbGetTargetUnit) :!label _label
          _
          (else
            (CallFunction|CheckNearestUnits)
            (Variables|Default|SetbGetTargetUnit true)
            (Default|UpdateGLASSCodefromEachFunc (Variables|Default|GetREF_%20InteractPanel))))
        (CallFunction|GotoTargetUnit)))
    (else
      (goto _label))))

(fn DragViaInput
  (bind _returnvalue (Game|GetPlayerController 0))
  (bind _triggermousepivot (Variables|Default|GetTriggerMousePivot))
  (bind _sm_mixer_move_handle (Variables|Default|GetSM_Mixer_Move_Handle))
  (bind _worldlocation (Game|Player|ConvertMouseLocationToWorldSpace _returnvalue))
  (bind _relativelocation (Variables|/Script/Engine.SceneComponent|GetRelativeLocation _sm_mixer_move_handle))
  (bind _screenlocation (Class|PlayerController|ProjectWorldLocationtoScreen _returnvalue _worldlocation false))
  (if (!= (.y _screenlocation) (.y _triggermousepivot))
    (Variables|Default|SetbGetTargetUnit false)
    (if (< (.y _screenlocation) (.y _triggermousepivot))
      (LocalVariables|SetL_LimitedLocation -40.8)
      (if (not (Class|KismetMathLibrary|LinearColorIsNearEqual (Math|Conversions|ToLinearColor(Float) (.x (Variables|/Script/Engine.SceneComponent|GetRelativeLocation (Variables|Default|GetSM_Mixer_Move_Handle)))) (Math|Conversions|ToLinearColor(Float) (LocalVariables|GetL_LimitedLocation)) 0.0001))
        (Transformation|AddLocalOffset (Variables|Default|GetSM_Mixer_Move_Handle) (Math|Vector|MakeVector (* (Variables|Default|GetDefaultSpeed) -1.0) 0.0 0.0) false false)
        (if (<= (.x (Variables|/Script/Engine.SceneComponent|GetRelativeLocation (Variables|Default|GetSM_Mixer_Move_Handle))) (LocalVariables|GetL_LimitedLocation))
          (Transformation|SetRelativeLocation _sm_mixer_move_handle (Math|Vector|MakeVector (LocalVariables|GetL_LimitedLocation) (.y _relativelocation) (.z _relativelocation)) false false :!label _label)
          (Variables|Default|SetbHasUpdateMousePivot false)
          (if (not (Variables|Default|GetbMeshReachLimit))
            (Variables|Default|SetbMeshReachLimit true)
            (Audio|SpawnSoundAttached "/Game/Project/Audio/MetaSoundSource/SE/MSS_MetalLock_4.MSS_MetalLock_4" (Variables|Default|GetSM_Mixer_Move_Handle) "None" "0, 0, 0" "0, 0, 0" "KeepRelativeOffset" false 1.0 1.0 0.0 0 0)
            (Variables|Default|SetbSoundPlaying false)
            (CallFunction|StopContinuedSE (Variables|Default|GetAudioEnable_Handle)))
          (else
            (CallFunction|UpdateTriggerMousePivot :!label _label_2)
            (Variables|Default|SetbMeshReachLimit false)
            (if (not (Variables|Default|GetbSoundPlaying))
              (Variables|Default|SetbSoundPlaying true)
              (bind _returnvalue_2 (Audio|SpawnSoundAttached "/Game/Project/Audio/MetaSoundSource/SE/MSS_ScaleSlider_7.MSS_ScaleSlider_7" (Variables|Default|GetSM_Mixer_Move_Handle) "None" "0, 0, 0" "0, 0, 0" "KeepRelativeOffset" false 1.0 1.0 0.0 0 0))
              (Variables|Default|SetAudioEnable_Handle _returnvalue_2)))))
      (else
        (LocalVariables|SetL_LimitedLocation 36.0)
        (if (not (Class|KismetMathLibrary|LinearColorIsNearEqual (Math|Conversions|ToLinearColor(Float) (.x (Variables|/Script/Engine.SceneComponent|GetRelativeLocation (Variables|Default|GetSM_Mixer_Move_Handle)))) (Math|Conversions|ToLinearColor(Float) (LocalVariables|GetL_LimitedLocation)) 0.0001))
          (Transformation|AddLocalOffset (Variables|Default|GetSM_Mixer_Move_Handle) (Math|Vector|MakeVector (Variables|Default|GetDefaultSpeed) 0.0 0.0) false false)
          (if (>= (.x (Variables|/Script/Engine.SceneComponent|GetRelativeLocation (Variables|Default|GetSM_Mixer_Move_Handle))) (LocalVariables|GetL_LimitedLocation))
            (goto _label)
            (else
              (goto _label_2))))))))

(fn FinishRemainOffset
  (params (bGoingOpen :type Boolean)))

(fn GotoTargetUnit
  (bind _sm_mixer_move_handle (Variables|Default|GetSM_Mixer_Move_Handle))
  (bind _sm_mixer_move_handle_2 (Variables|Default|GetSM_Mixer_Move_Handle))
  (bind _relativelocation (Variables|/Script/Engine.SceneComponent|GetRelativeLocation _sm_mixer_move_handle_2))
  (bind _relativelocation_2 (Variables|/Script/Engine.SceneComponent|GetRelativeLocation _sm_mixer_move_handle))
  (Utilities|FlowControl|Sequence
    (:then_0
      (Transformation|SetRelativeLocation (Variables|Default|GetSM_Mixer_Move_Handle) (Math|Interpolation|VInterpTo (Variables|/Script/Engine.SceneComponent|GetRelativeLocation _sm_mixer_move_handle_2) (Math|Vector|MakeVector (Variables|Default|GetTargetUnitsPosX) (.y _relativelocation) (.z _relativelocation)) (Utilities|Time|GetWorldDeltaSeconds) 4.0) false false))
    (:then_1
      (if (<= (Math|Float|Absolute(Float) (- (.x (Variables|/Script/Engine.SceneComponent|GetRelativeLocation (Variables|Default|GetSM_Mixer_Move_Handle))) (Variables|Default|GetTargetUnitsPosX))) 0.2)
        (Transformation|SetRelativeLocation _sm_mixer_move_handle (Math|Vector|MakeVector (Variables|Default|GetTargetUnitsPosX) (.y _relativelocation_2) (.z _relativelocation_2)) false false)
        (Variables|Default|SetbHasUpdateMousePivot false)
        (if (not (Variables|Default|GetbMeshReachLimit))
          (Variables|Default|SetbMeshReachLimit true)
          (Audio|SpawnSoundAttached "/Game/Project/Audio/MetaSoundSource/SE/MSS_MetalLock_4.MSS_MetalLock_4" (Variables|Default|GetSM_Mixer_Move_Handle) "None" "0, 0, 0" "0, 0, 0" "KeepRelativeOffset" false 1.0 1.0 0.0 0 0)
          (Variables|Default|SetbSoundPlaying false)
          (CallFunction|StopContinuedSE (Variables|Default|GetAudioEnable_Handle)))))))

(fn ReceiveGLASScode
  (params (Code :type Integer))
  (bind _output_get (Variables|Default|SetInsertedGLASSUnits Code))
  (Variables|Default|SetTargetUnitsPosX (Utilities|Array|Get(acopy) (Variables|Default|GetUnits) _output_get))
  (Variables|Default|SetbGetTargetUnit true)
  (Variables|Default|SetbHasInsertedGLASS true)
  (Default|UpdateGLASSCodefromEachFunc (Variables|Default|GetREF_%20InteractPanel)))

(fn UpdateTriggerMousePivot
  (bind _returnvalue (Game|GetPlayerController 0))
  (Variables|Default|SetTriggerMousePivot (.ScreenLocation (Class|PlayerController|ProjectWorldLocationtoScreen _returnvalue (.WorldLocation (Game|Player|ConvertMouseLocationToWorldSpace _returnvalue)) false))))