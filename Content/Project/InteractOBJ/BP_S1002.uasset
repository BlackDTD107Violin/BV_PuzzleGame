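; BP_S1002 is an interactable with clickable wardrobe doors and a two-stage drag puzzle: a lock, then a cover.
; Tick runs the active stage, rotating its pivot with vertical mouse movement and playing slide and finish sounds.
; Releasing past a threshold eases the pivot to completion with RInterpTo.
; Door clicks only set drag flags; door rotation is unfinished, and nothing here sets the lock or cover drag flags true.
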(event OnClicked(Wardrobe_Door_L)
  (params (TouchedComponent :type Primitive%20Component%20Object%20Reference) (ButtonPressed :type Key%20Structure :default "None"))
  (Variables|Default|SetbIsDraggingLDoor true)
  (Variables|/Game/ProjectDefault/FirstPerson/Blueprints/BP_FirstPersonCharacter.BP_FirstPersonCharacter_C|SetCurrentInteract (Variables|Default|GetPlayer) self))

(event OnClicked(Wardrobe_Door_R)
  (params (TouchedComponent :type Primitive%20Component%20Object%20Reference) (ButtonPressed :type Key%20Structure :default "None"))
  (Variables|Default|SetbIsDraggingRDoor true)
  (Variables|/Game/ProjectDefault/FirstPerson/Blueprints/BP_FirstPersonCharacter.BP_FirstPersonCharacter_C|SetCurrentInteract (Variables|Default|GetPlayer) self))

(event EventBeginPlay
  (bind _returnvalue (Game|GetPlayerController 0))
  (|CallParentFunction)
  (bind _asbp_first_person_character (Utilities|Casting|CastToBP_FirstPersonCharacter (Game|GetPlayerCharacter 0)))
  (Variables|Default|SetPlayer _asbp_first_person_character)
  (Input|EnableInput _returnvalue)
  (Variables|/Script/Engine.PlayerController|SetbEnableClickEvents _returnvalue true)
  (Variables|/Script/Engine.PlayerController|SetbEnableMouseOverEvents _returnvalue true))

(event EventTick
  (params (DeltaSeconds :type Float%20%28single-precision%29))
  (if (Variables|Default|GetbLockIsFinish)
    (if (not (Variables|Default|GetbCoverIsFinish))
      (CallFunction|CheckCoverState))
    (else
      (CallFunction|CheckLockState))))

(event EventInteractEnd
  (CallFunction|CancelingDrag)
  (Variables|/Game/ProjectDefault/FirstPerson/Blueprints/BP_FirstPersonCharacter.BP_FirstPersonCharacter_C|SetCurrentInteract (Variables|Default|GetPlayer) self)
  (Variables|Default|SetbSoundPlaying false))

(fn ConstructionScript
  (|CallParentFunction))

(fn UpdateTriggerMousePivot
  (bind _returnvalue (Game|GetPlayerController 0))
  (Variables|Default|SetTriggerMousePivot (.ScreenLocation (Class|PlayerController|ProjectWorldLocationtoScreen _returnvalue (.WorldLocation (Game|Player|ConvertMouseLocationToWorldSpace _returnvalue)) false))))

(fn DragLockViaInput
  (bind _returnvalue (Game|GetPlayerController 0))
  (bind _triggermousepivot (Variables|Default|GetTriggerMousePivot))
  (bind _worldlocation (Game|Player|ConvertMouseLocationToWorldSpace _returnvalue))
  (bind _screenlocation (Class|PlayerController|ProjectWorldLocationtoScreen _returnvalue _worldlocation false))
  (if (not (Variables|Default|GetbLockIsFinish))
    (if (!= (.y _screenlocation) (.y _triggermousepivot))
      (if (> (.y _screenlocation) (.y _triggermousepivot))
        (Transformation|AddLocalRotation (Variables|Default|GetLockPivot) (Math|Rotator|MakeRotator (Variables|Default|GetRotateSpeed) 0.0 0.0) false false)
        (if (>= (.roll (Variables|/Script/Engine.SceneComponent|GetRelativeRotation (Variables|Default|GetLockPivot))) 0.0)
          (Transformation|SetRelativeRotation (Variables|Default|GetLockPivot) "0, 0, 0" false false)
          (else
            (CallFunction|UpdateTriggerMousePivot)
            (if (not (Variables|Default|GetbSoundPlaying))
              (Variables|Default|SetbSoundPlaying true)
              (Audio|SpawnSoundAttached "/Game/Project/Audio/MetaSoundSource/MSS_S0003_LockSlide.MSS_S0003_LockSlide" (Variables|Default|GetLockPivot) "None" "0, 0, 0" "0, 0, 0" "KeepRelativeOffset" false 1.0 1.0 0.0 0 0))))
        (else
          (Transformation|AddLocalRotation (Variables|Default|GetLockPivot) (Math|Rotator|MakeRotator (* (Variables|Default|GetRotateSpeed) -1.0) 0.0 0.0) false false)
          (if (<= (Class|KismetMathLibrary|ClampAxis (.roll (Variables|/Script/Engine.SceneComponent|GetRelativeRotation (Variables|Default|GetLockPivot)))) 1.8e+02)
            (Variables|Default|SetbLockIsFinish true)
            (CallFunction|CancelingDrag)
            (Audio|SpawnSoundAttached "/Game/Project/Audio/MetaSoundSource/MSS_S0003_LockFinish.MSS_S0003_LockFinish" (Variables|Default|GetLockPivot) "None" "0, 0, 0" "0, 0, 0" "KeepRelativeOffset" false 1.0 1.0 0.0 0 0)
            (Variables|Default|SetbSoundPlaying false)
            (else
              (CallFunction|UpdateTriggerMousePivot)
              (if (not (Variables|Default|GetbSoundPlaying))
                (Variables|Default|SetbSoundPlaying true)
                (Audio|SpawnSoundAttached "/Game/Project/Audio/MetaSoundSource/MSS_S0003_LockSlide.MSS_S0003_LockSlide" (Variables|Default|GetLockPivot) "None" "0, 0, 0" "0, 0, 0" "KeepRelativeOffset" false 1.0 1.0 0.0 0 0)))))))))

(fn DragCoverViaInput
  (bind _returnvalue (Game|GetPlayerController 0))
  (bind _triggermousepivot (Variables|Default|GetTriggerMousePivot))
  (bind _worldlocation (Game|Player|ConvertMouseLocationToWorldSpace _returnvalue))
  (bind _screenlocation (Class|PlayerController|ProjectWorldLocationtoScreen _returnvalue _worldlocation false))
  (if (not (Variables|Default|GetbCoverIsFinish))
    (if (!= (.y _screenlocation) (.y _triggermousepivot))
      (if (> (.y _screenlocation) (.y _triggermousepivot))
        (Transformation|AddLocalRotation (Variables|Default|GetCoverPivot) (Math|Rotator|MakeRotator (Variables|Default|GetRotateSpeed) 0.0 0.0) false false)
        (if (>= (.roll (Variables|/Script/Engine.SceneComponent|GetRelativeRotation (Variables|Default|GetCoverPivot))) 0.0)
          (Transformation|SetRelativeRotation (Variables|Default|GetCoverPivot) "0, 0, 0" false false)
          (else
            (CallFunction|UpdateTriggerMousePivot)
            (if (not (Variables|Default|GetbSoundPlaying))
              (Variables|Default|SetbSoundPlaying true)
              (Audio|SpawnSoundAttached "/Game/Project/Audio/MetaSoundSource/MSS_S0003_CoverSlide.MSS_S0003_CoverSlide" (Variables|Default|GetCoverPivot) "None" "0, 0, 0" "0, 0, 0" "KeepRelativeOffset" false 1.0 1.0 0.0 0 0))))
        (else
          (Transformation|AddLocalRotation (Variables|Default|GetCoverPivot) (Math|Rotator|MakeRotator (* (Variables|Default|GetRotateSpeed) -1.0) 0.0 0.0) false false)
          (if (<= (Class|KismetMathLibrary|ClampAxis (.roll (Variables|/Script/Engine.SceneComponent|GetRelativeRotation (Variables|Default|GetCoverPivot)))) 2.7e+02)
            (Variables|Default|SetbCoverIsFinish true)
            (CallFunction|CancelingDrag)
            (Collision|SetCollisionProfileName (Variables|Default|GetStaticMesh) "TRICKignore" true :!class /Script/Engine.PrimitiveComponent)
            (Audio|SpawnSoundAttached "/Game/Project/Audio/MetaSoundSource/MSS_S0003_CoverFinish.MSS_S0003_CoverFinish" (Variables|Default|GetCoverPivot) "None" "0, 0, 0" "0, 0, 0" "KeepRelativeOffset" false 1.0 1.0 0.0 0 0)
            (Variables|Default|SetbSoundPlaying false)
            (else
              (CallFunction|UpdateTriggerMousePivot)
              (if (not (Variables|Default|GetbSoundPlaying))
                (Variables|Default|SetbSoundPlaying true)
                (Audio|SpawnSoundAttached "/Game/Project/Audio/MetaSoundSource/MSS_S0003_CoverSlide.MSS_S0003_CoverSlide" (Variables|Default|GetCoverPivot) "None" "0, 0, 0" "0, 0, 0" "KeepRelativeOffset" false 1.0 1.0 0.0 0 0)))))))))

(fn CancelingDrag
  (Variables|Default|SetbIsDraggingLock false)
  (Variables|Default|SetbIsDraggingCover false)
  (Variables|Default|SetbHasUpdateMousePivot false))

(fn FinishRemainingAngleLock
  (bind _lockpivot (Variables|Default|GetLockPivot))
  (bind _lockpivot_2 (Variables|Default|GetLockPivot))
  (bind _relativerotation (Variables|/Script/Engine.SceneComponent|GetRelativeRotation _lockpivot))
  (bind _relativerotation_2 (Variables|/Script/Engine.SceneComponent|GetRelativeRotation _lockpivot_2))
  (Utilities|FlowControl|Sequence
    (:then_0
      (Transformation|SetRelativeRotation (Variables|Default|GetLockPivot) (Math|Interpolation|RInterpTo (Variables|/Script/Engine.SceneComponent|GetRelativeRotation (Variables|Default|GetLockPivot)) (Math|Rotator|MakeRotator -1.8e+02 (.pitch _relativerotation) (.yaw _relativerotation)) (Utilities|Time|GetWorldDeltaSeconds) 4.0) false false))
    (:then_1
      (if (<= (.roll (Variables|/Script/Engine.SceneComponent|GetRelativeRotation (Variables|Default|GetLockPivot))) -179.0)
        (Transformation|SetRelativeRotation (Variables|Default|GetLockPivot) (Math|Rotator|MakeRotator -1.8e+02 (.pitch _relativerotation_2) (.yaw _relativerotation_2)) false false)
        (Variables|Default|SetbLockIsFinish true)
        (CallFunction|CancelingDrag)
        (Audio|SpawnSoundAttached "/Game/Project/Audio/MetaSoundSource/MSS_S0003_LockFinish.MSS_S0003_LockFinish" (Variables|Default|GetLockPivot) "None" "0, 0, 0" "0, 0, 0" "KeepRelativeOffset" false 1.0 1.0 0.0 0 0)
        (Variables|Default|SetbSoundPlaying false)))))

(fn FinishRemainingAngleCover
  (bind _coverpivot (Variables|Default|GetCoverPivot))
  (bind _coverpivot_2 (Variables|Default|GetCoverPivot))
  (bind _relativerotation (Variables|/Script/Engine.SceneComponent|GetRelativeRotation _coverpivot_2))
  (bind _relativerotation_2 (Variables|/Script/Engine.SceneComponent|GetRelativeRotation _coverpivot))
  (Utilities|FlowControl|Sequence
    (:then_0
      (Transformation|SetRelativeRotation (Variables|Default|GetCoverPivot) (Math|Interpolation|RInterpTo (Variables|/Script/Engine.SceneComponent|GetRelativeRotation (Variables|Default|GetCoverPivot)) (Math|Rotator|MakeRotator -9e+01 (.pitch _relativerotation) (.yaw _relativerotation)) (Utilities|Time|GetWorldDeltaSeconds) 4.0) false false))
    (:then_1
      (if (<= (.roll (Variables|/Script/Engine.SceneComponent|GetRelativeRotation (Variables|Default|GetCoverPivot))) -89.0)
        (Transformation|SetRelativeRotation (Variables|Default|GetCoverPivot) (Math|Rotator|MakeRotator -9e+01 (.pitch _relativerotation_2) (.yaw _relativerotation_2)) false false)
        (Variables|Default|SetbCoverIsFinish true)
        (CallFunction|CancelingDrag)
        (Collision|SetCollisionProfileName (Variables|Default|GetStaticMesh) "TRICKignore" true :!class /Script/Engine.PrimitiveComponent)
        (Audio|SpawnSoundAttached "/Game/Project/Audio/MetaSoundSource/MSS_S0003_CoverFinish.MSS_S0003_CoverFinish" (Variables|Default|GetCoverPivot) "None" "0, 0, 0" "0, 0, 0" "KeepRelativeOffset" false 1.0 1.0 0.0 0 0)
        (Variables|Default|SetbSoundPlaying false)))))

(fn CheckCoverState
  (if (Variables|Default|GetbIsDraggingCover)
    (if (Variables|Default|GetbHasUpdateMousePivot)
      (CallFunction|DragCoverViaInput)
      (else
        (Variables|Default|SetbHasUpdateMousePivot true)
        (CallFunction|UpdateTriggerMousePivot)))
    (elif (<= (.roll (Variables|/Script/Engine.SceneComponent|GetRelativeRotation (Variables|Default|GetCoverPivot))) -6e+01)
      (CallFunction|FinishRemainingAngleCover))))

(fn CheckLockState
  (if (Variables|Default|GetbIsDraggingLock)
    (if (Variables|Default|GetbHasUpdateMousePivot)
      (CallFunction|DragLockViaInput)
      (else
        (Variables|Default|SetbHasUpdateMousePivot true)
        (CallFunction|UpdateTriggerMousePivot)))
    (elif (<= (.roll (Variables|/Script/Engine.SceneComponent|GetRelativeRotation (Variables|Default|GetLockPivot))) -9e+01)
      (CallFunction|FinishRemainingAngleLock))))

(fn CheckLeftDoorState
  (if (Variables|Default|GetbIsDraggingLock)
    (if (Variables|Default|GetbHasUpdateMousePivot)
      (CallFunction|DragLockViaInput)
      (else
        (Variables|Default|SetbHasUpdateMousePivot true)
        (CallFunction|UpdateTriggerMousePivot)))
    (elif (<= (.roll (Variables|/Script/Engine.SceneComponent|GetRelativeRotation (Variables|Default|GetLockPivot))) -9e+01)
      (CallFunction|FinishRemainingAngleLock))))