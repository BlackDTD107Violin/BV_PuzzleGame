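; BP_GLASSItem is an inspectable glass item that can be taken out of notches on the mixer, calculate and final machines.
; Entering the inspector hides the mesh via ACItemComponent and, if the glass is inserted, clears it from its input or output notch, updating that machine's state.
; Exiting hides the actor and disables its collision.
; Three dynamic diamond materials, created at BeginPlay, are switched on by SetInheritDiamond to match the glass's inherit layer.
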(event EventBeginPlay
  (|CallParentFunction)
  (CallFunction|CreateDiamondMat))

(event EventEnterInspector
  (Default|SpawnSEandSetMeshHidden (Variables|Default|GetAC_ItemComponent) (Variables|Default|GetStaticMesh) true)
  (bind _currentinsertedta (Variables|Default|GetCurrentInsertedTA)
    (:then
      (bind _side (Default|PickOutGlass _currentinsertedta))
      (if (Utilities|Enum|Equal(Enum) _side "NewEnumerator3")
        (CallFunction|RemovefromOutputSide)
        (else
          (CallFunction|RemovefromInputSide))))
    (:else)))

(event EventExitInspector
  (Default|SpawnSEandSetMeshHidden (Variables|Default|GetAC_ItemComponent) (Variables|Default|GetStaticMesh) false)
  (Rendering|SetActorHiddenInGame true)
  (Collision|SetActorEnableCollision false))

(fn ConstructionScript
  (|CallParentFunction))

(fn RemovefromInputSide
  (switch Utilities|FlowControl|Switch|SwitchonE_SideState (Variables|/Game/Project/InteractOBJ/BP_OBJ_TA.BP_OBJ_TA_C|GetGlassTAside (Variables|Default|GetCurrentInsertedTA))
    (:NewEnumerator1
      (Default|RemoveGlassTAside (Variables|/Game/Project/InteractOBJ/BP_OBJ_TA.BP_OBJ_TA_C|GetREF%20GlassNotch (Variables|Default|GetCurrentInsertedTA)) (Variables|/Game/Project/InteractOBJ/BP_OBJ_TA.BP_OBJ_TA_C|GetGlassTAside (Variables|Default|GetCurrentInsertedTA)) :!label _label))
    (:NewEnumerator2
      (goto _label))
    (:NewEnumerator4
      (Default|UpdateGLASSCode (Variables|/Game/Project/InteractOBJ/BP_OBJ_TA.BP_OBJ_TA_C|GetREF%20GlassNotch (Variables|Default|GetCurrentInsertedTA))))
    (:NewEnumerator6
      (Variables|/Game/Project/InteractOBJ/BP_S9009.BP_S9009_C|SetbGlassCodeIsMatch (Variables|/Game/Project/InteractOBJ/BP_S9007.BP_S9007_C|GetREF_FinalMachine (Variables|/Game/Project/InteractOBJ/BP_OBJ_TA.BP_OBJ_TA_C|GetREF%20GlassNotch (Variables|Default|GetCurrentInsertedTA))) false)))
  (Variables|/Game/Project/InteractOBJ/BP_S9007.BP_S9007_C|SetREF_InsertedGLASS (Variables|/Game/Project/InteractOBJ/BP_OBJ_TA.BP_OBJ_TA_C|GetREF%20GlassNotch (Variables|Default|GetCurrentInsertedTA)) 0)
  (Variables|Default|SetCurrentInsertedTA 0)
  (Default|CallConsumeThisGlass self))

(fn RemovefromOutputSide
  (Utilities|IsValid (Variables|/Game/Project/InteractOBJ/BP_S9007.BP_S9007_C|GetREF_MainMachine (Variables|/Game/Project/InteractOBJ/BP_OBJ_TA.BP_OBJ_TA_C|GetREF%20GlassNotch (Variables|Default|GetCurrentInsertedTA)))
    (:Is%20Valid
      (Variables|/Game/Project/InteractOBJ/BP_S9001.BP_S9001_C|SetbMixNotchIsEmpty (Variables|/Game/Project/InteractOBJ/BP_S9007.BP_S9007_C|GetREF_MainMachine (Variables|/Game/Project/InteractOBJ/BP_OBJ_TA.BP_OBJ_TA_C|GetREF%20GlassNotch (Variables|Default|GetCurrentInsertedTA))) true)
      (Variables|Default|SetCurrentInsertedTA 0)
      (Default|CallConsumeThisGlass self))))

(fn CreateDiamondMat
  (Utilities|FlowControl|Sequence
    (:then_0
      (bind _returnvalue (Rendering|Material|CreateDynamicMaterialInstance "/Game/Project/Artist/KeyObj/Material/Slider_Diamond00.Slider_Diamond00" "None" "None" :!class /Script/Engine.KismetMaterialLibrary))
      (Utilities|Array|Add (Variables|Default|GetDiamondGroups) _returnvalue))
    (:then_1
      (bind _returnvalue_2 (Rendering|Material|CreateDynamicMaterialInstance "/Game/Project/Artist/KeyObj/Material/Slider_Diamond02.Slider_Diamond02" "None" "None" :!class /Script/Engine.KismetMaterialLibrary))
      (Utilities|Array|Add (Variables|Default|GetDiamondGroups) _returnvalue_2))
    (:then_2
      (bind _returnvalue_3 (Rendering|Material|CreateDynamicMaterialInstance "/Game/Project/Artist/KeyObj/Material/Slider_Diamond01.Slider_Diamond01" "None" "None" :!class /Script/Engine.KismetMaterialLibrary))
      (Utilities|Array|Add (Variables|Default|GetDiamondGroups) _returnvalue_3))
    (:then_3
      (for _array_element (Variables|Default|GetDiamondGroups)
        (Rendering|Material|SetScalarParameterValue _array_element "Enable" 0.0 :!class /Script/Engine.MaterialInstanceDynamic)
        (Rendering|Material|SetScalarParameterValue _array_element "Speed" 0.0 :!class /Script/Engine.MaterialInstanceDynamic)))))

(fn SetInheritDiamond
  (LocalVariables|SetL_Layer (.inheritlayer (Variables|Default|GetThisGlass)))
  (for _index (range 0 2)
    (bind _output_get (LocalVariables|SetL_LoopIndex _index))
    (if (< _output_get (LocalVariables|GetL_Layer))
      (Rendering|Material|SetScalarParameterValue (Utilities|Array|Get(acopy) (Variables|Default|GetDiamondGroups) (LocalVariables|GetL_LoopIndex)) "Enable" 1.0 :!class /Script/Engine.MaterialInstanceDynamic)
      (Rendering|Material|SetScalarParameterValue (Utilities|Array|Get(acopy) (Variables|Default|GetDiamondGroups) (LocalVariables|GetL_LoopIndex)) "Speed" 0.1 :!class /Script/Engine.MaterialInstanceDynamic)
      (else
        (Rendering|Material|SetScalarParameterValue (Utilities|Array|Get(acopy) (Variables|Default|GetDiamondGroups) (LocalVariables|GetL_LoopIndex)) "Enable" 0.0 :!class /Script/Engine.MaterialInstanceDynamic)
        (Rendering|Material|SetScalarParameterValue (Utilities|Array|Get(acopy) (Variables|Default|GetDiamondGroups) (LocalVariables|GetL_LoopIndex)) "Speed" 0.0 :!class /Script/Engine.MaterialInstanceDynamic)))
    (Rendering|Material|SetMaterial (Variables|Default|GetStaticMesh) (+ (LocalVariables|GetL_LoopIndex) 4) (Utilities|Array|Get(acopy) (Variables|Default|GetDiamondGroups) (LocalVariables|GetL_LoopIndex)))))