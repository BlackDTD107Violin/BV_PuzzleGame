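; Interactable object that rotates its Cube while the left mouse button is held on it.
; BeginPlay enables input, click and mouse-over events on the player controller and caches the first-person character.
; Clicking PressedTA sets IsPressed and registers the object as the character's CurrentPressed; releasing or CancelPressed clears the flag.
; Tick eases the Cube's roll toward MaxAngle while pressed and back to InitAngle otherwise, using RInterpTo.
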(event OnClicked(PressedTA)
  (params (TouchedComponent :type Primitive%20Component%20Object%20Reference) (ButtonPressed :type Key%20Structure :default "None"))
  (Development|PrintString "Clicked")
  (Variables|Default|SetbIsPressed true)
  (Variables|/Game/ProjectDefault/FirstPerson/Blueprints/BP_FirstPersonCharacter.BP_FirstPersonCharacter_C|SetCurrentPressed (Variables|Default|GetPlayer) self))

(event OnReleased(PressedTA)
  (params (TouchedComponent :type Primitive%20Component%20Object%20Reference) (ButtonReleased :type Key%20Structure :default "None"))
  (Development|PrintString "Clicked")
  (Variables|Default|SetbIsPressed false))

(event EventBeginPlay
  (bind _returnvalue (Game|GetPlayerController 0))
  (|CallParentFunction)
  (Input|EnableInput _returnvalue)
  (Variables|/Script/Engine.PlayerController|SetbEnableClickEvents _returnvalue true)
  (Variables|/Script/Engine.PlayerController|SetbEnableMouseOverEvents _returnvalue true)
  (bind _asbp_first_person_character (Utilities|Casting|CastToBP_FirstPersonCharacter (Game|GetPlayerCharacter 0)))
  (Variables|Default|SetPlayer _asbp_first_person_character))

(event EventTick
  (params (DeltaSeconds :type Float%20%28single-precision%29))
  (bind _cube (Variables|Default|GetCube))
  (bind _cube_2 (Variables|Default|GetCube))
  (bind _relativerotation (Variables|/Script/Engine.SceneComponent|GetRelativeRotation _cube_2))
  (bind _relativerotation_2 (Variables|/Script/Engine.SceneComponent|GetRelativeRotation _cube))
  (if (Variables|Default|GetbIsPressed)
    (Transformation|SetRelativeRotation (Variables|Default|GetCube) (Math|Interpolation|RInterpTo (Variables|/Script/Engine.SceneComponent|GetRelativeRotation (Variables|Default|GetCube)) (Math|Rotator|MakeRotator (Variables|Default|GetMaxAngle) (.pitch _relativerotation) (.yaw _relativerotation)) (Utilities|Time|GetWorldDeltaSeconds) 1.0) false false)
    (else
      (Transformation|SetRelativeRotation (Variables|Default|GetCube) (Math|Interpolation|RInterpTo (Variables|/Script/Engine.SceneComponent|GetRelativeRotation (Variables|Default|GetCube)) (Math|Rotator|MakeRotator (Variables|Default|GetInitAngle) (.pitch _relativerotation_2) (.yaw _relativerotation_2)) (Utilities|Time|GetWorldDeltaSeconds) 1.0) false false))))

(event EventCancelPressed
  (Variables|Default|SetbIsPressed false)
  (Development|PrintString "Call Success"))

(fn ConstructionScript
  (|CallParentFunction))