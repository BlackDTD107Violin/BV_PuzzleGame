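; Interactable glass notch, a socket used within the mix, extract and calculate glass machines, which it identifies from its parent actor.
; Interacting blends the camera to the notch, locks player input and swaps trigger collision so the child BP_OBJ_TA is clickable only while empty.
; Mix or extract results become pooled glass items placed in the notch.
; Inserted glass is attached and tracked, and the vertical-suffixed calculate machine variant (_V) is notified.
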(event EventBeginPlay
  (bind _returnvalue (Game|GetPlayerController 0))
  (bind _returnvalue_2 (Actor|GetParentActor))
  (|CallParentFunction)
  (Utilities|FlowControl|Sequence
    (:then_0
      (bind _asbp_first_person_character (Utilities|Casting|CastToBP_FirstPersonCharacter (Game|GetPlayerCharacter 0)))
      (Variables|Default|SetPlayer _asbp_first_person_character)
      (Input|EnableInput _returnvalue)
      (Variables|/Script/Engine.PlayerController|SetbEnableClickEvents _returnvalue true)
      (Variables|/Script/Engine.PlayerController|SetbEnableMouseOverEvents _returnvalue true))
    (:then_1
      (bind _asbp_obj_ta (Utilities|Casting|CastToBP_OBJ_TA (Variables|/Script/Engine.ChildActorComponent|GetChildActor (Variables|Default|GetGLASS_TA))))
      (bind _output_get (Variables|Default|SetREF_OBJ%20TA _asbp_obj_ta))
      (Collision|SetCollisionProfileName (Variables|/Game/Project/InteractOBJ/BP_OBJ_TA.BP_OBJ_TA_C|GetKey_TriggerArea _output_get) "NoCollision" true :!class /Script/Engine.PrimitiveComponent)
      (Utilities|IsValid _returnvalue_2
        (:Is%20Valid
          (bind _asbp_glass_mix_machine (Utilities|Casting|CastToBP_GlassMixMachine _returnvalue_2)
            (:then
              (Variables|Default|SetREF_GlassMixMachine _asbp_glass_mix_machine)
              (Variables|Default|SetbIsMixMachine true))
            (:CastFailed
              (bind _asbp_extract_machine (Utilities|Casting|CastToBP_ExtractMachine (Actor|GetParentActor))
                (:then
                  (Variables|Default|SetREF_Extract%20Machine _asbp_extract_machine))
                (:CastFailed
                  (bind _asbp_glass_calculate_machine (Utilities|Casting|CastToBP_GlassCalculateMachine (Actor|GetParentActor)))
                  (Variables|Default|SetREF_GlassCalculateMachine _asbp_glass_calculate_machine))))))))))

(event EventZoomin
  (params (ZoomComponent :type Actor%20Component%20Object%20Reference))
  (bind _returnvalue (Game|GetPlayerController 0))
  (Game|Player|SetViewTargetwithBlend (Game|GetPlayerController 0) self 0.5 "VTBlend_Linear" 0.0 true)
  (Input|SetIgnoreMoveInput _returnvalue true)
  (Input|SetIgnoreLookInput _returnvalue true)
  (Default|ClearGamePromptUIView (Variables|Default|GetPlayer))
  (Collision|SetCollisionProfileName (Variables|Default|GetZoomTrigger_Main) "NoCollision" true :!class /Script/Engine.PrimitiveComponent)
  (if (> (Utilities|Array|Length (Variables|Default|GetSETLists)) 0)
    (Collision|SetCollisionProfileName (Variables|/Game/Project/InteractOBJ/BP_OBJ_TA.BP_OBJ_TA_C|GetKey_TriggerArea (Variables|Default|GetREF_OBJ%20TA)) "NoCollision" true :!class /Script/Engine.PrimitiveComponent)
    (else
      (Collision|SetCollisionProfileName (Variables|/Game/Project/InteractOBJ/BP_OBJ_TA.BP_OBJ_TA_C|GetKey_TriggerArea (Variables|Default|GetREF_OBJ%20TA)) "BlockAllDynamic" true :!class /Script/Engine.PrimitiveComponent))))

(event EventZoomOut
  (bind _returnvalue (Game|GetPlayerController 0))
  (Game|Player|SetViewTargetwithBlend (Game|GetPlayerController 0) (Game|GetPlayerCharacter 0) 0.5 "VTBlend_Linear" 0.0 true)
  (Input|ResetIgnoreMoveInput _returnvalue)
  (Input|ResetIgnoreLookInput _returnvalue)
  (Utilities|FlowControl|Delay 0.5)
  (Collision|SetCollisionProfileName (Variables|Default|GetZoomTrigger_Main) "BlockAllDynamic" true :!class /Script/Engine.PrimitiveComponent)
  (Collision|SetCollisionProfileName (Variables|/Game/Project/InteractOBJ/BP_OBJ_TA.BP_OBJ_TA_C|GetKey_TriggerArea (Variables|Default|GetREF_OBJ%20TA)) "NoCollision" true :!class /Script/Engine.PrimitiveComponent))

(event EventInteract
  (params (InteractActor :type Actor%20Object%20Reference) (InteractTarget :type Actor%20Component%20Object%20Reference))
  (CallFunction|Zoomin InteractTarget))

(fn ConstructionScript
  (|CallParentFunction))

(fn UpdateGLASSCode
  (if (Variables|Default|GetbIsMixMachine)
    (bind _updatedglass (Default|ReturnUpdatedGLASSCode (Variables|Default|GetREF_GlassMixMachine)))
    (Variables|/Game/Project/InteractOBJ/BP_GLASSItem.BP_GLASSItem_C|SetThisGlass (Variables|Default|GetREF_InsertedGLASS) _updatedglass)
    (else
      (bind _updatedglass_2 (Default|ReturnUpdatedGLASSCode (Variables|Default|GetREF_GlassCalculateMachine)))
      (Variables|/Game/Project/InteractOBJ/BP_GLASSItem.BP_GLASSItem_C|SetThisGlass (Variables|Default|GetREF_InsertedGLASS) _updatedglass_2))))

(fn ReturnGlassTAside
  (bind _asbp_obj_ta (Utilities|Casting|CastToBP_OBJ_TA (Variables|/Script/Engine.ChildActorComponent|GetChildActor (Variables|Default|GetGLASS_TA))))
  (return (Variables|/Game/Project/InteractOBJ/BP_OBJ_TA.BP_OBJ_TA_C|GetGlassTAside _asbp_obj_ta)))

(fn SetupGlassTAside
  (params (GlassTAside :type E_SideState%20Enum :default "NewEnumerator0"))
  (bind _asbp_obj_ta (Utilities|Casting|CastToBP_OBJ_TA (Variables|/Script/Engine.ChildActorComponent|GetChildActor (Variables|Default|GetGLASS_TA))))
  (Variables|/Game/Project/InteractOBJ/BP_OBJ_TA.BP_OBJ_TA_C|SetGlassTAside _asbp_obj_ta GlassTAside))

(fn RemoveGlassTAside
  (params (Side :type E_SideState%20Enum :default "NewEnumerator0"))
  (Default|EraseTotemPreviewer (Variables|Default|GetREF_GlassMixMachine) Side))

(fn ReceiveMixDataandCreate
  (params (GlassUnite :type ST%20Glass%20Base%20Collection%20Structure))
  (Variables|Default|SetCurrentGLASS GlassUnite)
  (Utilities|FlowControl|Sequence
    (:then_0
      (bind _glassfrompool (Default|AcquireGlassfromPool (Variables|Default|GetREF_GlassPool)))
      (bind _output_get (LocalVariables|SetL_Temp_GLASSbase _glassfrompool))
      (Transformation|SetActorTransform _output_get (Math|Conversions|ToTransform(Vector) (Transformation|GetWorldLocation (Variables|Default|GetPlaceLocation))))
      (Variables|/Game/Project/InteractOBJ/BP_GLASSItem.BP_GLASSItem_C|SetThisGlass (LocalVariables|GetL_Temp_GLASSbase) (Utilities|Struct|MakeST_GlassBaseCollection (LocalVariables|GetL_Temp_GLASSbase) -1 (.inheritlayer (Variables|Default|GetCurrentGLASS)) (.preview (Variables|Default|GetCurrentGLASS)) (.glassvalue (Variables|Default|GetCurrentGLASS)) 0 0)))
    (:then_1
      (bind _asbp_obj_ta (Utilities|Casting|CastToBP_OBJ_TA (Variables|/Script/Engine.ChildActorComponent|GetChildActor (Variables|Default|GetGLASS_TA))))
      (Default|SetupNewGlass _asbp_obj_ta (LocalVariables|GetL_Temp_GLASSbase))
      (Collision|SetCollisionEnabled (Variables|/Game/Project/InteractOBJ/BP_OBJ_TA.BP_OBJ_TA_C|GetKey_TriggerArea _asbp_obj_ta) "NoCollision"))))

(fn ReceiveExtractDataandCreate
  (params (Data :type ST%20Glass%20Value%20Structure))
  (Variables|Default|SetCurrentExtractData Data)
  (Utilities|FlowControl|Sequence
    (:then_0
      (bind _glassfrompool (Default|AcquireGlassfromPool (Variables|Default|GetREF_GlassPool)))
      (bind _output_get (LocalVariables|SetL_Temp_GLASSbase _glassfrompool))
      (Transformation|SetActorTransform _output_get (Math|Conversions|ToTransform(Vector) (Transformation|GetWorldLocation (Variables|Default|GetPlaceLocation))))
      (Variables|/Game/Project/InteractOBJ/BP_GLASSItem.BP_GLASSItem_C|SetThisGlass (LocalVariables|GetL_Temp_GLASSbase) (Utilities|Struct|MakeST_GlassBaseCollection (LocalVariables|GetL_Temp_GLASSbase) -1 0 0 (Utilities|Array|MakeArray (Variables|Default|GetCurrentExtractData)) 0 0)))
    (:then_1
      (bind _asbp_obj_ta (Utilities|Casting|CastToBP_OBJ_TA (Variables|/Script/Engine.ChildActorComponent|GetChildActor (Variables|Default|GetGLASS_TA))))
      (Default|SetupNewGlass _asbp_obj_ta (LocalVariables|GetL_Temp_GLASSbase))
      (Collision|SetCollisionEnabled (Variables|/Game/Project/InteractOBJ/BP_OBJ_TA.BP_OBJ_TA_C|GetKey_TriggerArea _asbp_obj_ta) "NoCollision"))))

(fn SpawnGlassActor
  (params (GlassData :type BP%20Core%20OBJ%20GLASS%20Object%20Reference))
  (bind _asbp_glassitem (Utilities|Casting|CastToBP_GLASSItem GlassData))
  (bind _output_get (Variables|Default|SetREF_InsertedGLASS _asbp_glassitem))
  (Development|SetHiddeninGame (Variables|/Game/Project/Core/InteractOBJ/BP_CoreOBJ.BP_CoreOBJ_C|GetStaticMesh _output_get) false false)
  (Transformation|SetActorLocation (Variables|Default|GetREF_InsertedGLASS) (Transformation|GetWorldLocation (Variables|Default|GetPlaceLocation)) false false)
  (Transformation|AttachActorToActor (Variables|Default|GetREF_InsertedGLASS) self "None" "KeepWorld" "KeepRelative" "KeepRelative" true)
  (Utilities|Array|Add (Variables|Default|GetSETLists) (Variables|Default|GetREF_InsertedGLASS))
  (bind _asbp_glass_calculate_machine_v (Utilities|Casting|CastToBP_GlassCalculateMachine_V (Variables|Default|GetREF_GlassCalculateMachine)))
  (Default|GlassHasInserted _asbp_glass_calculate_machine_v (Variables|Default|GetREF_InsertedGLASS)))

(fn AcquireGlassfromPool
  (bind _ref_glasspool (Variables|Default|GetREF_GlassPool))
  (bind _glasspool (Variables|/Game/Project/Core/GameSystem/BP_GlassManager.BP_GlassManager_C|GetGlassPool _ref_glasspool))
  (bind _returnvalue (Utilities|Array|Length _glasspool))
  (if (> _returnvalue 0)
    (Variables|Default|SetMaxPool _returnvalue)
    (Utilities|IsValid (Utilities|Array|Get(acopy) _glasspool (Variables|Default|GetGlassIndex))
      (:Is%20Valid
        (bind _result (Math|Integer|IncrementInt (Variables|Default|GetGlassIndex))
          (:%20%20
            (bind _output_get (Variables|Default|SetGlassIndex _result))
            (if (== _output_get (Variables|Default|GetMaxPool))
              (Variables|Default|SetGlassIndex 0))
            (return (Utilities|Array|Get(acopy) _glasspool (Variables|Default|GetGlassIndex))))))
      (:Is%20Not%20Valid
        _)))
  (return 0))