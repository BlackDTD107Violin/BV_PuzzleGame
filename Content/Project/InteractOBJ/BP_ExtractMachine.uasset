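; BP_ExtractMachine is an interactable machine that turns an inserted object's extract data into output at a glass mix notch.
; On BeginPlay it registers itself with its child slider actor and caches its child input and output notch actors.
; ReceiveOBJExtractCode stores the inserted object, and CheckExtractRequest passes its data to the output notch when input is set, output is empty and no extraction runs, otherwise printing the reason.
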(event EventBeginPlay
  (|CallParentFunction)
  (Utilities|FlowControl|Sequence
    (:then_0
      (bind _asbp_t_mix_machine_slider (Utilities|Casting|CastToBP_T_MixMachineSlider (Variables|/Script/Engine.ChildActorComponent|GetChildActor (Variables|Default|GetSliderBar))))
      (Default|AssignExtractMachinetoChild _asbp_t_mix_machine_slider self))
    (:then_1
      (CallFunction|PresetEachNotch))))

(fn ConstructionScript
  (|CallParentFunction))

(fn CheckExtractRequest
  (if (Math|Boolean|ANDBoolean (Variables|Default|GetbOBJNotchIsSet) (not (Variables|Default|GetbIsExtracting)) (Variables|Default|GetbMixNotchIsEmpty))
    (Default|ReceiveExtractDataandCreate (Variables|Default|GetOutput%20Notch) (Utilities|Struct|BreakST_ItemCollection (Variables|Default|GetOBJExtractData)))
    (Variables|Default|SetbMixNotchIsEmpty false)
    (elif (Variables|Default|GetbIsExtracting)
      (Development|PrintString "During Extracting")
      (elif (Variables|Default|GetbMixNotchIsEmpty)
        (Development|PrintString "OBJ Notch Is Empty")
        (else
          (Development|PrintString "Mix Notch Has Glass"))))))

(fn PresetEachNotch
  (Utilities|FlowControl|Sequence
    (:then_0
      (bind _asbp_objnotch (Utilities|Casting|CastToBP_OBJNotch (Variables|/Script/Engine.ChildActorComponent|GetChildActor (Variables|Default|GetExtractNotch))))
      (Variables|Default|SetOBJInputNotch _asbp_objnotch))
    (:then_1
      (bind _asbp_glass_mix_notch (Utilities|Casting|CastToBP_GlassMixNotch (Variables|/Script/Engine.ChildActorComponent|GetChildActor (Variables|Default|GetGLASSNotch_Mix))))
      (bind _output_get (Variables|Default|SetOutput%20Notch _asbp_glass_mix_notch))
      (Default|SetupMixNotchSide _output_get "NewEnumerator3"))))

(fn ReceiveOBJExtractCode
  (params (InsertedOBJ :type ST%20Item%20Collection%20Structure))
  (Variables|Default|SetOBJExtractData InsertedOBJ)
  (Variables|Default|SetbOBJNotchIsSet true))