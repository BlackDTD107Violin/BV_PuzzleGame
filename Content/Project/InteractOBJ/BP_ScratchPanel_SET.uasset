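; Scratch-off panel actor where mouse input erases a seal layer over a base layer through a render-target mask.
; Construction creates dynamic erase materials and the render target, which is cleared on BeginPlay and drawn with the mask material every Tick.
; When the cursor enters the mesh while erasing, a trace's hit UV, scaled by mouse position, updates the mask.
; A separate paint-seal scratch path exists, but its material creation is unwired.
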(event OnClicked(StaticMesh)
  (params (TouchedComponent :type Primitive%20Component%20Object%20Reference) (ButtonPressed :type Key%20Structure :default "None"))
  (Variables|Default|Setb_IsErasing true))

(event OnBeginCursorOver(StaticMesh)
  (params (TouchedComponent :type Primitive%20Component%20Object%20Reference))
  (bind _returnvalue (Game|GetPlayerController 0))
  (bind (_worldlocation _worlddirection) (Game|Player|ConvertMouseLocationToWorldSpace _returnvalue))
  (if (Variables|Default|Getb_IsErasing)
    (bind (_outhit _returnvalue_2) (Collision|LineTraceByChannel _worldlocation (+ _worldlocation (* _worlddirection 1e+03)) "TraceTypeQuery1" true 0 "None"))
    (if _returnvalue_2
      (CallFunction|SetParams (.UV (Class|GameplayStatics|FindCollisionUV _outhit))))))

(event OnReleased(StaticMesh)
  (params (TouchedComponent :type Primitive%20Component%20Object%20Reference) (ButtonReleased :type Key%20Structure :default "None"))
  (Variables|Default|Setb_IsErasing false))

(event OnEndCursorOver(StaticMesh)
  (params (TouchedComponent :type Primitive%20Component%20Object%20Reference)))

(event Custom|ScratchOnBoard
  (params (LocationToScratch :type Vector%202D%20Structure))
  (bind _returnvalue (Game|GetPlayerController 0))
  (bind _returnvalue_2 (Math|Conversions|ToVector(Vector2D) LocationToScratch 0.01))
  (bind (_x _y _z) (Math|Vector|BreakVector _returnvalue_2))
  (bind (_locationx _locationy) (Game|Player|GetMousePosition _returnvalue))
  (Rendering|Material|SetVectorParameterValue (Variables|Default|GetM_PaintSeal) "ScratchLocation" (Math|Conversions|ToLinearColor(Vector) (Math|Vector|MakeVector (* _x (/ _locationx 384.0)) (* _y (/ _locationy 384.0)) _z)) :!class /Script/Engine.MaterialInstanceDynamic)
  (Rendering|DrawMaterialtoRenderTarget "/Game/Project/InteractOBJ/CRT_ScratchBoard.CRT_ScratchBoard" (Variables|Default|GetM_PaintSeal)))

(event Custom|ScratchSize
  (params (ScratchSize :type Float%20%28double-precision%29))
  (Rendering|Material|SetScalarParameterValue (Variables|Default|GetM_PaintSeal) "Size" ScratchSize :!class /Script/Engine.MaterialInstanceDynamic))

(event Custom|Set%20Params
  (params (EraseUV :type Vector%202D%20Structure))
  (bind _returnvalue (Game|GetPlayerController 0))
  (bind (_x _y) (Math|Vector2D|BreakVector2D EraseUV))
  (bind (_locationx _locationy) (Game|Player|GetMousePosition _returnvalue))
  (Rendering|Material|SetVectorParameterValue (Variables|Default|GetM_EraseMask) "ParamP" (Utilities|Struct|MakeLinearColor (* _x (/ _locationx 384.0)) (* _y (/ _locationy 384.0)) 0.0 1.0) :!class /Script/Engine.MaterialInstanceDynamic)
  (Rendering|Material|SetTextureParameterValue (Variables|Default|GetM_EraseBase) "Param" (Variables|Default|GetRenderTarget))
  (Rendering|Material|SetTextureParameterValue (Variables|Default|GetM_EraseSeal) "Param" (Variables|Default|GetRenderTarget)))

(event EventBeginPlay
  (|CallParentFunction)
  (Rendering|ClearRenderTarget2D (Variables|Default|GetRenderTarget)))

(event EventTick
  (params (DeltaSeconds :type Float%20%28single-precision%29))
  (Rendering|DrawMaterialtoRenderTarget (Variables|Default|GetRenderTarget) (Variables|Default|GetM_EraseMask)))

(fn ConstructionScript
  (|CallParentFunction)
  (Utilities|FlowControl|Sequence
    (:then_0
      (bind _returnvalue (Rendering|Material|CreateDynamicMaterialInstance "/Game/Project/MaterialLibrary/M_EraseBase.M_EraseBase" "None" "None" :!class /Script/Engine.KismetMaterialLibrary))
      (bind _output_get (Variables|Default|SetM_EraseBase _returnvalue))
      (Rendering|Material|SetMaterial (Variables|Default|GetPlane1) 0 _output_get))
    (:then_1
      (bind _returnvalue_2 (Rendering|Material|CreateDynamicMaterialInstance "/Game/Project/MaterialLibrary/M_EraseSeal.M_EraseSeal" "None" "None" :!class /Script/Engine.KismetMaterialLibrary))
      (bind _output_get_2 (Variables|Default|SetM_EraseSeal _returnvalue_2))
      (Rendering|Material|SetMaterial (Variables|Default|GetPlane) 0 _output_get_2))
    (:then_2
      (bind _returnvalue_3 (Rendering|Material|CreateDynamicMaterialInstance "/Game/Project/MaterialLibrary/M_EraseMask.M_EraseMask" "None" "None" :!class /Script/Engine.KismetMaterialLibrary))
      (Variables|Default|SetM_EraseMask _returnvalue_3)
      (bind _returnvalue_4 (Rendering|CreateRenderTarget2D 256 256 "RTF_RGBA16f"))
      (Variables|Default|SetRenderTarget _returnvalue_4))))