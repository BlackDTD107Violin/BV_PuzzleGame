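; BP_Extract_TA is an insertion slot for the extract machine, expected to have a BP_SET_OBJplace_ExtractMachine as its parent actor, which it caches on BeginPlay.
; RefreshInsertedOBJ passes the inserted object's data to the linked extract machine and calls Interact on the parent with the item actor.
; It then unhides the item, enables its collision, flags the slot occupied and registers itself on the item if it is a pickup or key.
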(event EventBeginPlay
  (bind _asbp_set_objplace_extract_machine (Utilities|Casting|CastToBP_SET_OBJplace_ExtractMachine (Actor|GetParentActor)))
  (Variables|Default|SetREF%20SET%20OBJplace%20Extract%20Machine _asbp_set_objplace_extract_machine))

(fn ConstructionScript)

(fn RefreshInsertedOBJ
  (params (InsertedOBJ :type ST%20Item%20Collection%20Structure))
  (Variables|Default|SetInsertedOBJ InsertedOBJ)
  (Default|ReceiveOBJExtractCode (Variables|/Game/Project/InteractOBJ/BP_SET_OBJplace_ExtractMachine.BP_SET_OBJplace_ExtractMachine_C|GetREF_OBJExtractMachine (Variables|Default|GetREF%20SET%20OBJplace%20Extract%20Machine)) (Variables|Default|GetInsertedOBJ))
  (Default|Interact (Variables|Default|GetREF%20SET%20OBJplace%20Extract%20Machine) (.TargetItemActor (Utilities|Struct|BreakST_ItemCollection (Variables|Default|GetInsertedOBJ))))
  (Rendering|SetActorHiddenInGame (.TargetItemActor (Utilities|Struct|BreakST_ItemCollection (Variables|Default|GetInsertedOBJ))) false)
  (Collision|SetActorEnableCollision (.TargetItemActor (Utilities|Struct|BreakST_ItemCollection (Variables|Default|GetInsertedOBJ))) true)
  (Variables|Default|SetbExtractTAIsEmpty false)
  (bind _asbp_core_obj_pickup (Utilities|Casting|CastToBP_CoreOBJ_PICKUP (.TargetItemActor (Utilities|Struct|BreakST_ItemCollection (Variables|Default|GetInsertedOBJ))))
    (:then
      (Variables|/Game/Project/Core/InteractOBJ/BP_CoreOBJ_PICKUP.BP_CoreOBJ_PICKUP_C|SetCurrentInsertedExtractTA_Old _asbp_core_obj_pickup self))
    (:CastFailed
      (bind _asbp_core_obj_key (Utilities|Casting|CastToBP_CoreOBJ_KEY (.TargetItemActor (Utilities|Struct|BreakST_ItemCollection (Variables|Default|GetInsertedOBJ)))))
      (Variables|/Game/Project/Core/InteractOBJ/BP_CoreOBJ_KEY.BP_CoreOBJ_KEY_C|SetCurrentInsertedExtractTA_Old _asbp_core_obj_key self))))