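; Interactable extractor puzzle machine that turns an inserted object's extract data into a glass in its result notch.
; Zoom triggers blend the view to per-part camera points and toggle collision on triggers and parts.
; Unlocking the candle via key K1002 plays an activation sequence and, with an object set, enables the mouse-dragged switch handle.
; A full throw creates the result and plays a sequence; Tick eases handle and slide back while the result is empty.
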(event OnClicked(SM_Extractor_Switch_Handle_Cube)
  (params (TouchedComponent :type Primitive%20Component%20Object%20Reference) (ButtonPressed :type Key%20Structure :default "None"))
  (Variables|Default|SetbIsDragSlider true)
  (Variables|/Game/ProjectDefault/FirstPerson/Blueprints/BP_FirstPersonCharacter.BP_FirstPersonCharacter_C|SetCurrentInteract (Variables|Default|GetPlayer) self))

(event EventBeginPlay
  (bind _returnvalue (Game|GetPlayerController 0))
  (bind _sk_extractor (Variables|Default|GetSK_Extractor))
  (|CallParentFunction)
  (Utilities|FlowControl|Sequence
    (:then_0
      (bind _asbp_first_person_character (Utilities|Casting|CastToBP_FirstPersonCharacter (Game|GetPlayerCharacter 0)))
      (Variables|Default|SetPlayer _asbp_first_person_character)
      (Input|EnableInput _returnvalue)
      (Variables|/Script/Engine.PlayerController|SetbEnableClickEvents _returnvalue true)
      (Variables|/Script/Engine.PlayerController|SetbEnableMouseOverEvents _returnvalue true)
      (Components|Animation|PlayAnimation _sk_extractor "/Game/Project/Artist/Machine/Mesh/SK_Extractor_Anim_Two_Side_Anim_Sun_SideAction.SK_Extractor_Anim_Two_Side_Anim_Sun_SideAction" false)
      (Audio|Components|Audio|Stop _sk_extractor))
    (:then_1
      (CallFunction|PresetValue)
      (CallFunction|PresetZoomGroup))))

(event EventInteractiveUnlocked
  (params (AttachKEY :type Actor%20Object%20Reference) (MatchOBJCode :type Name :default "None"))
  (Variables|Default|SetbCandleIsSet true)
  (Audio|SpawnSoundatLocation "/Game/Project/Audio/MetaSoundSource/MSS_S0002_OpenDoor.MSS_S0002_OpenDoor" (Transformation|GetWorldLocation (Variables|Default|GetSM_Extractor_Candle)) "0, 0, 0" 1.0 1.0 0.0 0 0)
  (bind _outactor (Sequencer|Player|CreateLevelSequencePlayer "/Game/Project/LS_ExtractMachine_Activate.LS_ExtractMachine_Activate" (Utilities|Struct|MakeMovieSceneSequencePlaybackSettings false "(Value=0)" 1.0 0.0 false false true true false false false false)))
  (Development|PrintString (Utilities|String|Append "Activate Seq = " (Utilities|GetDisplayName _outactor)) true true "(R=0.000000,G=0.660000,B=1.000000,A=1.000000)" 15.0)
  (Sequencer|Player|Play (Variables|/Script/LevelSequence.LevelSequenceActor|GetSequencePlayer _outactor) :!class /Script/MovieScene.MovieSceneSequencePlayer))

(event EventTick
  (params (DeltaSeconds :type Float%20%28single-precision%29))
  (if (Variables|Default|GetbIsStandBy)
    (if (Variables|Default|GetbResultIsEmpty)
      (CallFunction|SwitchHandle-BacktoDefault)
      (CallFunction|CoSlide-BacktoDefault))
    (else
      (switch int (Variables|Default|GetZoomInPart)
        (:1
          (if (Math|Boolean|ANDBoolean (Variables|Default|GetbCandleIsSet) (Variables|Default|GetbOBJIsSet) (Variables|Default|GetbResultIsEmpty))
            (CallFunction|CheckState-SwitchHandle)))
        (:3
          (if (Variables|Default|GetbResultIsEmpty)
            (CallFunction|SwitchHandle-BacktoDefault)
            (CallFunction|CoSlide-BacktoDefault)))))))

(event EventZoomin
  (params (ZoomComponent :type Actor%20Component%20Object%20Reference))
  (bind _returnvalue (Game|GetPlayerController 0))
  (bind _biszoomset (CallFunction|AssignZoomPosition ZoomComponent))
  (if _biszoomset
    (Game|Player|SetViewTargetwithBlend (Game|GetPlayerController 0) self 0.5 "VTBlend_Linear" 0.0 true)
    (Input|SetIgnoreMoveInput _returnvalue true)
    (Input|SetIgnoreLookInput _returnvalue true)
    (Default|ClearGamePromptUIView (Variables|Default|GetPlayer))
    (CallFunction|SwitchTACollisionProfile false)))

(event EventInteract
  (params (InteractActor :type Actor%20Object%20Reference) (InteractTarget :type Actor%20Component%20Object%20Reference))
  (CallFunction|Zoomin InteractTarget))

(event EventInteractEnd
  (Variables|/Game/ProjectDefault/FirstPerson/Blueprints/BP_FirstPersonCharacter.BP_FirstPersonCharacter_C|SetCurrentInteract (Variables|Default|GetPlayer) self)
  (Variables|Default|SetbSoundPlaying false)
  (switch int (Variables|Default|GetZoomInPart)
    (:1
      (Variables|Default|SetbIsDragSlider false))))

(event EventZoomOut
  (bind _returnvalue (Game|GetPlayerController 0))
  (Game|Player|SetViewTargetwithBlend (Game|GetPlayerController 0) (Game|GetPlayerCharacter 0) 0.5 "VTBlend_Linear" 0.0 true)
  (CallFunction|SwitchMeshCollisionProfile false)
  (Input|ResetIgnoreMoveInput _returnvalue)
  (Input|ResetIgnoreLookInput _returnvalue)
  (Variables|Default|SetbIsStandBy true)
  (Utilities|FlowControl|Delay 0.5)
  (CallFunction|SwitchTACollisionProfile true))

(fn ConstructionScript
  (|CallParentFunction))

(fn AssignZoomPosition
  (params (ZoomInComponent :type Object%20Object%20Reference))
  (bind (_array_element _array_index) (Utilities|Array|ForEachLoopwithBreak (Variables|Default|GetGroupWidgetTrigger) :!label _label)
    (:LoopBody
      (if (== _array_element ZoomInComponent)
        (Variables|Default|SetZoomInPart _array_index)
        (goto _label Break)))
    (:Completed
      (Transformation|SetRelativeTransform (Variables|Default|GetZoomInCamera) (Utilities|Array|Get(acopy) (Variables|Default|GetZoomInPoint) (Variables|Default|GetZoomInPart)) false false)
      (CallFunction|SwitchMeshCollisionProfile true)
      (Variables|Default|SetbIsStandBy false)
      (return true))))

(fn CheckExtractRequest
  (if (and (Variables|Default|GetbOBJIsSet) (Variables|Default|GetbResultIsEmpty))
    (Default|ReceiveExtractDataandCreate (Variables|Default|GetREF_ResultNotch) (Utilities|Struct|BreakST_ItemCollection (Variables|Default|GetOBJExtractData)))
    (Variables|Default|SetbResultIsEmpty false)
    (bind _outactor (Sequencer|Player|CreateLevelSequencePlayer "/Game/Project/LS_ExtractMachine_Create.LS_ExtractMachine_Create" (Utilities|Struct|MakeMovieSceneSequencePlaybackSettings true "(Value=0)" 1.0 0.0 false false true true false false false false)))
    (Sequencer|Player|Play (Variables|/Script/LevelSequence.LevelSequenceActor|GetSequencePlayer _outactor) :!class /Script/MovieScene.MovieSceneSequencePlayer)
    (EventDispatchers|BindEventtoOnFinished (Variables|/Script/LevelSequence.LevelSequenceActor|GetSequencePlayer _outactor) (EventDispatchers|CreateEvent :!event CoSlide-PopOut))
    (elif (Variables|Default|GetbResultIsEmpty)
      (Development|PrintString "OBJ Notch Is Empty")
      (else
        (Development|PrintString "Mix Notch Has Glass")))))

(fn CheckState-SwitchHandle
  (if (Variables|Default|GetbIsDragSlider)
    (if (Variables|Default|GetbHasUpdateMousePivot)
      (CallFunction|SwitchHandle-DragViaInput)
      (else
        (Variables|Default|SetbHasUpdateMousePivot true)
        (CallFunction|UpdateTriggerMousePivot)))
    (else
      (CallFunction|SwitchHandle-FinishRemainAngle (>= (.roll (Variables|/Script/Engine.SceneComponent|GetRelativeRotation (Variables|Default|GetSM_Extractor_Switch_Handle))) 175.0)))))

(fn CoSlide-BacktoDefault
  (bind _sm_extractor_co_slide_bottom (Variables|Default|GetSM_Extractor_Co-slide_Bottom))
  (bind _sm_extractor_co_slide_bottom_2 (Variables|Default|GetSM_Extractor_Co-slide_Bottom))
  (bind _relativelocation (Variables|/Script/Engine.SceneComponent|GetRelativeLocation _sm_extractor_co_slide_bottom_2))
  (bind _relativelocation_2 (Variables|/Script/Engine.SceneComponent|GetRelativeLocation _sm_extractor_co_slide_bottom))
  (LocalVariables|SetL_TargetPos 179.264749)
  (LocalVariables|SetL_TouchPos 180.264749)
  (Utilities|FlowControl|Sequence
    (:then_0
      (Transformation|SetRelativeLocation (Variables|Default|GetSM_Extractor_Co-slide_Bottom) (Math|Interpolation|VInterpTo (Variables|/Script/Engine.SceneComponent|GetRelativeLocation (Variables|Default|GetSM_Extractor_Co-slide_Bottom)) (Math|Vector|MakeVector (.x _relativelocation_2) (.y _relativelocation_2) (LocalVariables|GetL_TargetPos)) (Utilities|Time|GetWorldDeltaSeconds) 4.0) false false))
    (:then_1
      (if (<= (.z (Variables|/Script/Engine.SceneComponent|GetRelativeLocation (Variables|Default|GetSM_Extractor_Co-slide_Bottom))) (LocalVariables|GetL_TouchPos))
        (Transformation|SetRelativeLocation _sm_extractor_co_slide_bottom_2 (Math|Vector|MakeVector (.x _relativelocation) (.y _relativelocation) (LocalVariables|GetL_TargetPos)) false false)
        (if (not (Variables|Default|GetbMeshReachLimit))
          (Variables|Default|SetbMeshReachLimit true)
          (Audio|SpawnSoundAttached "/Game/Project/Audio/MetaSoundSource/MSS_S0003_LockFinish.MSS_S0003_LockFinish" (Variables|Default|GetSM_Extractor_Co-slide_Bottom) "None" "0, 0, 0" "0, 0, 0" "KeepRelativeOffset" false 1.0 1.0 0.0 0 0)
          (Variables|Default|SetbSoundPlaying false))))))

(fn CoSlide-PopOut
  (bind _sm_extractor_co_slide_bottom (Variables|Default|GetSM_Extractor_Co-slide_Bottom))
  (bind _relativelocation (Variables|/Script/Engine.SceneComponent|GetRelativeLocation _sm_extractor_co_slide_bottom))
  (LocalVariables|SetL_TargetPos 214.264749)
  (LocalVariables|SetL_TouchPos 213.264749)
  (Transformation|SetRelativeLocation _sm_extractor_co_slide_bottom (Math|Vector|MakeVector (.x _relativelocation) (.y _relativelocation) (LocalVariables|GetL_TargetPos)) false false))

(fn ExtractGlass
  (if (Variables|Default|GetbResultIsEmpty)
    (Variables|Default|SetbResultIsEmpty false)
    (Development|PrintString "The Moment of Start Extract film")))

(fn PresetValue
  (Utilities|FlowControl|Sequence
    (:then_0
      (bind _asbp_obj_ta (Utilities|Casting|CastToBP_OBJ_TA (Variables|/Script/Engine.ChildActorComponent|GetChildActor (Variables|Default|GetKEY_TA))))
      (Variables|/Game/Project/InteractOBJ/BP_OBJ_TA.BP_OBJ_TA_C|SetKEY_MatchCode _asbp_obj_ta "K1002")
      (Default|PresetNotchValue _asbp_obj_ta "NewEnumerator0"))
    (:then_1
      (bind _asbp_s9007 (Utilities|Casting|CastToBP_S9007 (Variables|/Script/Engine.ChildActorComponent|GetChildActor (Variables|Default|GetOBJNotch))))
      (Variables|Default|SetREF_OBJNotch _asbp_s9007))
    (:then_2
      (bind _asbp_s9007_2 (Utilities|Casting|CastToBP_S9007 (Variables|/Script/Engine.ChildActorComponent|GetChildActor (Variables|Default|GetExtractorerResultNotch))))
      (bind _output_get (Variables|Default|SetREF_ResultNotch _asbp_s9007_2))
      (Default|SetupGlassTAside _output_get "NewEnumerator3")
      (Variables|/Game/Project/InteractOBJ/BP_S9007.BP_S9007_C|SetREF_GlassPool (Variables|Default|GetREF_ResultNotch) (Variables|Default|GetREF_GlassPool)))))

(fn PresetZoomGroup
  (Utilities|Array|Add (Variables|Default|GetGroupWidgetTrigger) (Variables|Default|GetWidget%20Trigger_BackTable))
  (Utilities|Array|Add (Variables|Default|GetGroupWidgetTrigger) (Variables|Default|GetWidget%20Trigger_SwitchHandle))
  (Utilities|Array|Add (Variables|Default|GetGroupWidgetTrigger) (Variables|Default|GetWidget%20Trigger_Candle))
  (Utilities|Array|Add (Variables|Default|GetGroupWidgetTrigger) (Variables|Default|GetWidget%20Trigger_ExtractResult)))

(fn ReceiveOBJExtractCode
  (params (InsertedOBJ :type ST%20Item%20Collection%20Structure))
  (Variables|Default|SetOBJExtractData InsertedOBJ)
  (Variables|Default|SetbOBJIsSet true))

(fn SwitchHandle-BacktoDefault
  (bind _sm_extractor_switch_handle (Variables|Default|GetSM_Extractor_Switch_Handle))
  (bind _sm_extractor_switch_handle_2 (Variables|Default|GetSM_Extractor_Switch_Handle))
  (bind _relativerotation (Variables|/Script/Engine.SceneComponent|GetRelativeRotation _sm_extractor_switch_handle_2))
  (bind _relativerotation_2 (Variables|/Script/Engine.SceneComponent|GetRelativeRotation _sm_extractor_switch_handle))
  (Utilities|FlowControl|Sequence
    (:then_0
      (Transformation|SetRelativeRotation (Variables|Default|GetSM_Extractor_Switch_Handle) (Math|Rotator|Lerp(Rotator) (Variables|/Script/Engine.SceneComponent|GetRelativeRotation (Variables|Default|GetSM_Extractor_Switch_Handle)) (Math|Rotator|MakeRotator 0.1 (.pitch _relativerotation) (.yaw _relativerotation)) 0.03 true) false false))
    (:then_1
      (if (<= (.roll (Variables|/Script/Engine.SceneComponent|GetRelativeRotation (Variables|Default|GetSM_Extractor_Switch_Handle))) 1.0)
        (Transformation|SetRelativeRotation (Variables|Default|GetSM_Extractor_Switch_Handle) (Math|Rotator|MakeRotator 0.0 (.pitch _relativerotation_2) (.yaw _relativerotation_2)) false false)
        (Variables|Default|SetbHasUpdateMousePivot false)
        (if (not (Variables|Default|GetbMeshReachLimit))
          (Variables|Default|SetbMeshReachLimit true)
          (Audio|SpawnSoundAttached "/Game/Project/Audio/MetaSoundSource/MSS_S0003_LockFinish.MSS_S0003_LockFinish" (Variables|Default|GetSM_Extractor_Switch_Handle) "None" "0, 0, 0" "0, 0, 0" "KeepRelativeOffset" false 1.0 1.0 0.0 0 0)
          (Variables|Default|SetbSoundPlaying false))))))

(fn SwitchHandle-DragViaInput
  (bind _returnvalue (Game|GetPlayerController 0))
  (bind _triggermousepivot (Variables|Default|GetTriggerMousePivot))
  (bind _sm_extractor_switch_handle (Variables|Default|GetSM_Extractor_Switch_Handle))
  (bind _worldlocation (Game|Player|ConvertMouseLocationToWorldSpace _returnvalue))
  (bind _relativerotation (Variables|/Script/Engine.SceneComponent|GetRelativeRotation _sm_extractor_switch_handle))
  (bind _screenlocation (Class|PlayerController|ProjectWorldLocationtoScreen _returnvalue _worldlocation false))
  (if (!= (.y _screenlocation) (.y _triggermousepivot))
    (if (> (.y _screenlocation) (.y _triggermousepivot))
      (LocalVariables|SetL_LimitedAngle 1.8e+02)
      (Transformation|AddLocalRotation (Variables|Default|GetSM_Extractor_Switch_Handle) (Math|Rotator|MakeRotator (Variables|Default|GetSliderSpeed) 0.0 0.0) false false)
      (if (>= (Class|KismetMathLibrary|ClampAxis (.roll (Variables|/Script/Engine.SceneComponent|GetRelativeRotation (Variables|Default|GetSM_Extractor_Switch_Handle)))) (LocalVariables|GetL_LimitedAngle))
        (Transformation|SetRelativeRotation _sm_extractor_switch_handle (Math|Rotator|MakeRotator (LocalVariables|GetL_LimitedAngle) (.pitch _relativerotation) (.yaw _relativerotation)) false false :!label _label)
        (Variables|Default|SetbHasUpdateMousePivot false)
        (if (== (LocalVariables|GetL_LimitedAngle) 1.8e+02)
          (CallFunction|CheckExtractRequest)
          (if (not (Variables|Default|GetbMeshReachLimit))
            (Variables|Default|SetbMeshReachLimit true)
            (Audio|SpawnSoundAttached "/Game/Project/Audio/MetaSoundSource/MSS_S0003_LockFinish.MSS_S0003_LockFinish" (Variables|Default|GetSM_Extractor_Switch_Handle) "None" "0, 0, 0" "0, 0, 0" "KeepRelativeOffset" false 1.0 1.0 0.0 0 0)
            (Variables|Default|SetbSoundPlaying false)))
        (else
          (CallFunction|UpdateTriggerMousePivot :!label _label_2)
          (Variables|Default|SetbMeshReachLimit false)
          (if (not (Variables|Default|GetbSoundPlaying))
            (Variables|Default|SetbSoundPlaying true)
            (Audio|SpawnSoundAttached "/Game/Project/Audio/MetaSoundSource/MSS_S0003_LockSlide.MSS_S0003_LockSlide" (Variables|Default|GetSM_Extractor_Switch_Handle) "None" "0, 0, 0" "0, 0, 0" "KeepRelativeOffset" false 1.0 1.0 0.0 0 0))))
      (else
        (LocalVariables|SetL_LimitedAngle 0.0)
        (Transformation|AddLocalRotation (Variables|Default|GetSM_Extractor_Switch_Handle) (Math|Rotator|MakeRotator (* (Variables|Default|GetSliderSpeed) -1.0) 0.0 0.0) false false)
        (if (<= (.roll (Variables|/Script/Engine.SceneComponent|GetRelativeRotation (Variables|Default|GetSM_Extractor_Switch_Handle))) (LocalVariables|GetL_LimitedAngle))
          (goto _label)
          (else
            (goto _label_2)))))))

(fn SwitchHandle-FinishRemainAngle
  (params (bGoingActivate :type Boolean))
  (bind _sm_extractor_switch_handle (Variables|Default|GetSM_Extractor_Switch_Handle))
  (bind _sm_extractor_switch_handle_2 (Variables|Default|GetSM_Extractor_Switch_Handle))
  (bind _relativerotation (Variables|/Script/Engine.SceneComponent|GetRelativeRotation _sm_extractor_switch_handle))
  (bind _relativerotation_2 (Variables|/Script/Engine.SceneComponent|GetRelativeRotation _sm_extractor_switch_handle_2))
  (bind _output_get (LocalVariables|SetL_GoingActivate bGoingActivate))
  (if _output_get
    (LocalVariables|SetL_TargetAngle 1.8e+02)
    (LocalVariables|SetL_TouchAngle 179.0)
    (else
      (LocalVariables|SetL_TargetAngle 0.0)
      (LocalVariables|SetL_TouchAngle 1.0)))
  (Utilities|FlowControl|Sequence
    (:then_0
      (Transformation|SetRelativeRotation (Variables|Default|GetSM_Extractor_Switch_Handle) (Math|Interpolation|RInterpTo (Variables|/Script/Engine.SceneComponent|GetRelativeRotation _sm_extractor_switch_handle_2) (Math|Rotator|MakeRotator (LocalVariables|GetL_TargetAngle) (.pitch _relativerotation_2) (.yaw _relativerotation_2)) (Utilities|Time|GetWorldDeltaSeconds) 4.0) false false))
    (:then_1
      (if (and (LocalVariables|GetL_GoingActivate) (>= (.roll (Variables|/Script/Engine.SceneComponent|GetRelativeRotation (Variables|Default|GetSM_Extractor_Switch_Handle))) (LocalVariables|GetL_TouchAngle)))
        (CallFunction|CheckExtractRequest)
        (Transformation|SetRelativeRotation _sm_extractor_switch_handle (Math|Rotator|MakeRotator (LocalVariables|GetL_TargetAngle) (.pitch _relativerotation) (.yaw _relativerotation)) false false :!label _label)
        (Variables|Default|SetbHasUpdateMousePivot false)
        (if (not (Variables|Default|GetbMeshReachLimit))
          (Variables|Default|SetbMeshReachLimit true)
          (Audio|SpawnSoundAttached "/Game/Project/Audio/MetaSoundSource/MSS_S0003_LockFinish.MSS_S0003_LockFinish" (Variables|Default|GetSM_Extractor_Switch_Handle) "None" "0, 0, 0" "0, 0, 0" "KeepRelativeOffset" false 1.0 1.0 0.0 0 0)
          (Variables|Default|SetbSoundPlaying false))
        (elif (and (not (LocalVariables|GetL_GoingActivate)) (<= (.roll (Variables|/Script/Engine.SceneComponent|GetRelativeRotation (Variables|Default|GetSM_Extractor_Switch_Handle))) (LocalVariables|GetL_TouchAngle)))
          (goto _label))))))

(fn SwitchMeshCollisionProfile
  (params (bIsBlock :type Boolean))
  (bind _ref_objnotch (Variables|Default|GetREF_OBJNotch))
  (bind _ref_resultnotch (Variables|Default|GetREF_ResultNotch))
  (bind _ref_resultnotch_2 (Variables|Default|GetREF_ResultNotch))
  (bind _ref_objnotch_2 (Variables|Default|GetREF_OBJNotch))
  (bind _setlists (Variables|/Game/Project/Core/InteractOBJ/BP_CoreOBJ_SET.BP_CoreOBJ_SET_C|GetSETLists _ref_objnotch_2))
  (bind _setlists_2 (Variables|/Game/Project/Core/InteractOBJ/BP_CoreOBJ_SET.BP_CoreOBJ_SET_C|GetSETLists _ref_objnotch))
  (bind _setlists_3 (Variables|/Game/Project/Core/InteractOBJ/BP_CoreOBJ_SET.BP_CoreOBJ_SET_C|GetSETLists _ref_resultnotch))
  (bind _setlists_4 (Variables|/Game/Project/Core/InteractOBJ/BP_CoreOBJ_SET.BP_CoreOBJ_SET_C|GetSETLists _ref_resultnotch_2))
  (bind _output (Utilities|Array|Get(acopy) _setlists))
  (bind _output_2 (Utilities|Array|Get(acopy) _setlists_4))
  (bind _output_3 (Utilities|Array|Get(acopy) _setlists_3))
  (bind _output_4 (Utilities|Array|Get(acopy) _setlists_2))
  (if bIsBlock
    (switch int (Variables|Default|GetZoomInPart)
      (:0
        (Utilities|IsValid _output_4
          (:Is%20Valid
            (Collision|SetCollisionProfileName (Variables|/Game/Project/Core/InteractOBJ/BP_CoreOBJ.BP_CoreOBJ_C|GetStaticMesh _output_4) "BlockAllDynamic" true :!class /Script/Engine.PrimitiveComponent))))
      (:1
        (Collision|SetCollisionProfileName (Variables|Default|GetSM_Extractor_Switch_Handle_Cube) "BlockAllDynamic" true :!class /Script/Engine.PrimitiveComponent))
      (:3
        (Utilities|IsValid _output_3
          (:Is%20Valid
            (Collision|SetCollisionProfileName (Variables|/Game/Project/Core/InteractOBJ/BP_CoreOBJ.BP_CoreOBJ_C|GetStaticMesh _output_3) "BlockAllDynamic" true :!class /Script/Engine.PrimitiveComponent)))))
    (else
      (switch int (Variables|Default|GetZoomInPart)
        (:0
          (Utilities|IsValid _output
            (:Is%20Valid
              (Collision|SetCollisionProfileName (Variables|/Game/Project/Core/InteractOBJ/BP_CoreOBJ.BP_CoreOBJ_C|GetStaticMesh _output) "NoCollision" true :!class /Script/Engine.PrimitiveComponent))))
        (:1
          (Collision|SetCollisionProfileName (Variables|Default|GetSM_Extractor_Switch_Handle_Cube) "NoCollision" true :!class /Script/Engine.PrimitiveComponent))
        (:3
          (Utilities|IsValid _output_2
            (:Is%20Valid
              (Collision|SetCollisionProfileName (Variables|/Game/Project/Core/InteractOBJ/BP_CoreOBJ.BP_CoreOBJ_C|GetStaticMesh _output_2) "NoCollision" true :!class /Script/Engine.PrimitiveComponent))))))))

(fn SwitchTACollisionProfile
  (params (bIsBlock :type Boolean))
  (if bIsBlock
    (for _array_element (Variables|Default|GetGroupWidgetTrigger)
      (Collision|SetCollisionProfileName _array_element "BlockAllDynamic" true :!class /Script/Engine.PrimitiveComponent))
    (else
      (for _array_element_2 (Variables|Default|GetGroupWidgetTrigger)
        (Collision|SetCollisionProfileName _array_element_2 "NoCollision" true :!class /Script/Engine.PrimitiveComponent)))))

(fn UpdateTriggerMousePivot
  (bind _returnvalue (Game|GetPlayerController 0))
  (Variables|Default|SetTriggerMousePivot (.ScreenLocation (Class|PlayerController|ProjectWorldLocationtoScreen _returnvalue (.WorldLocation (Game|Player|ConvertMouseLocationToWorldSpace _returnvalue)) false))))

(fn PlayAnimMachineActivate
  (params (State :type Integer))
  (switch int State
    (:0
      (Components|Animation|PlayAnimation (Variables|Default|GetSK_Extractor) "/Game/Project/Artist/Machine/Mesh/SK_Extractor_Anim_Two_Side_Anim_Sun_SideAction.SK_Extractor_Anim_Two_Side_Anim_Sun_SideAction" false))
    (:1
      (Components|Animation|PlayAnimation (Variables|Default|GetSK_Extractor) "/Game/Project/Artist/Machine/Mesh/SK_Extractor_Anim_Two_Side_Anim_Moon_SideAction.SK_Extractor_Anim_Two_Side_Anim_Moon_SideAction" false))))