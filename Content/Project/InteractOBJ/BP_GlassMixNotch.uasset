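; BP_GlassMixNotch is an interactable glass slot that spawns glass made from mix or extract data.
; Both receive functions reach the GlassNotch child actor, spawn a BP_GLASS_BASEtest at its PlaceLocation, fill its glass struct, then register it with the nested BP_OBJ_TA and disable that key trigger's collision.
; Zoom events blend the view between notch and player, toggling input and mesh collision.
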(event EventBeginPlay
  (|CallParentFunction)
  (bind _asbp_first_person_character (Utilities|Casting|CastToBP_FirstPersonCharacter (Game|GetPlayerCharacter 0)))
  (Variables|Default|SetPlayer _asbp_first_person_character))

(event EventZoomin
  (bind _returnvalue (Game|GetPlayerController 0))
  (Game|Player|SetViewTargetwithBlend (Game|GetPlayerController 0) self 0.5 "VTBlend_Linear" 0.0 true)
  (Input|SetIgnoreMoveInput _returnvalue true)
  (Input|SetIgnoreLookInput _returnvalue true)
  (Default|ClearGamePromptUIView (Variables|Default|GetPlayer))
  (Collision|SetCollisionProfileName (Variables|Default|GetStaticMesh) "TRICKignore" true :!class /Script/Engine.PrimitiveComponent))

(event EventZoomOut
  (bind _returnvalue (Game|GetPlayerController 0))
  (Game|Player|SetViewTargetwithBlend (Game|GetPlayerController 0) (Game|GetPlayerCharacter 0) 0.5 "VTBlend_Linear" 0.0 true)
  (Input|ResetIgnoreMoveInput _returnvalue)
  (Input|ResetIgnoreLookInput _returnvalue)
  (Collision|SetCollisionProfileName (Variables|Default|GetStaticMesh) "BlockAllDynamic" true :!class /Script/Engine.PrimitiveComponent))

(fn ConstructionScript
  (|CallParentFunction))

(fn SetupMixNotchSide
  (params (Side :type E_SideState%20Enum :default "NewEnumerator0"))
  (bind _asbp_set_glassplace_mix_machine (Utilities|Casting|CastToBP_SET_GLASSplace_MixMachine (Variables|/Script/Engine.ChildActorComponent|GetChildActor (Variables|Default|GetGlassNotch))))
  (Default|SetupGlassTAside _asbp_set_glassplace_mix_machine Side))

(fn ReceiveMixDataandCreate
  (params (GlassUnite :type ST%20Glass%20Base%20Collection%20Structure))
  (Variables|Default|SetCurrentGLASS GlassUnite)
  (Utilities|FlowControl|Sequence
    (:then_0
      (bind _asbp_set_glassplace_mix_machine (Utilities|Casting|CastToBP_SET_GLASSplace_MixMachine (Variables|/Script/Engine.ChildActorComponent|GetChildActor (Variables|Default|GetGlassNotch))))
      (LocalVariables|SetL_SET_GLASSplaceMixMachine _asbp_set_glassplace_mix_machine))
    (:then_1
      (bind _returnvalue (Game|SpawnActorfromClass "/Game/Project/InteractOBJ/BP_GLASS_BASEtest.BP_GLASS_BASEtest_C" (Math|Conversions|ToTransform(Vector) (Transformation|GetWorldLocation (Variables|/Game/Project/InteractOBJ/BP_SET_GLASSplace_MixMachine.BP_SET_GLASSplace_MixMachine_C|GetPlaceLocation (LocalVariables|GetL_SET_GLASSplaceMixMachine)))) "Undefined" 0 "NewEnumerator1" false false 0))
      (bind _output_get (LocalVariables|SetL_tempGLASSbase _returnvalue))
      (Variables|/Game/Project/InteractOBJ/BP_GLASS_BASEtest.BP_GLASS_BASEtest_C|SetThisGlass _output_get (Utilities|Struct|MakeST_GlassBaseCollection _output_get -1 (.inheritlayer (Variables|Default|GetCurrentGLASS)) (.preview (Variables|Default|GetCurrentGLASS)) (.glassvalue (Variables|Default|GetCurrentGLASS)))))
    (:then_2
      (bind _asbp_obj_ta (Utilities|Casting|CastToBP_OBJ_TA (Variables|/Script/Engine.ChildActorComponent|GetChildActor (Variables|/Game/Project/InteractOBJ/BP_SET_GLASSplace_MixMachine.BP_SET_GLASSplace_MixMachine_C|GetGLASS_TA (LocalVariables|GetL_SET_GLASSplaceMixMachine)))))
      (Default|SetupNewGlass _asbp_obj_ta (LocalVariables|GetL_tempGLASSbase))
      (Collision|SetCollisionEnabled (Variables|/Game/Project/InteractOBJ/BP_OBJ_TA.BP_OBJ_TA_C|GetKey_TriggerArea _asbp_obj_ta) "NoCollision"))))

(fn ReceiveExtractDataandCreate
  (params (Data :type ST%20Glass%20Value%20Structure))
  (Variables|Default|SetCurrentExtractData Data)
  (Utilities|FlowControl|Sequence
    (:then_0
      (bind _asbp_set_glassplace_mix_machine (Utilities|Casting|CastToBP_SET_GLASSplace_MixMachine (Variables|/Script/Engine.ChildActorComponent|GetChildActor (Variables|Default|GetGlassNotch))))
      (LocalVariables|SetL_SET_GlassplaceExtractMachine _asbp_set_glassplace_mix_machine))
    (:then_1
      (bind _returnvalue (Game|SpawnActorfromClass "/Game/Project/InteractOBJ/BP_GLASS_BASEtest.BP_GLASS_BASEtest_C" (Math|Conversions|ToTransform(Vector) (Transformation|GetWorldLocation (Variables|/Game/Project/InteractOBJ/BP_SET_GLASSplace_MixMachine.BP_SET_GLASSplace_MixMachine_C|GetPlaceLocation (LocalVariables|GetL_SET_GlassplaceExtractMachine)))) "Undefined" 0 "NewEnumerator6" false false 0))
      (bind _output_get (LocalVariables|SetL_tempGLASSbase _returnvalue))
      (Variables|/Game/Project/InteractOBJ/BP_GLASS_BASEtest.BP_GLASS_BASEtest_C|SetThisGlass _output_get (Utilities|Struct|MakeST_GlassBaseCollection _output_get -1 0 "/Game/Developers/LinYanChen/Image/IMS_GlassBase.IMS_GlassBase" (Utilities|Array|MakeArray (Variables|Default|GetCurrentExtractData)))))
    (:then_2
      (bind _asbp_obj_ta (Utilities|Casting|CastToBP_OBJ_TA (Variables|/Script/Engine.ChildActorComponent|GetChildActor (Variables|/Game/Project/InteractOBJ/BP_SET_GLASSplace_MixMachine.BP_SET_GLASSplace_MixMachine_C|GetGLASS_TA (LocalVariables|GetL_SET_GlassplaceExtractMachine)))))
      (Default|SetupNewGlass _asbp_obj_ta (LocalVariables|GetL_tempGLASSbase))
      (Collision|SetCollisionEnabled (Variables|/Game/Project/InteractOBJ/BP_OBJ_TA.BP_OBJ_TA_C|GetKey_TriggerArea _asbp_obj_ta) "NoCollision"))))