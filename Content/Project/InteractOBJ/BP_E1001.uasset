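; BP_E1001 is an interactable, extractable object that uses the Meteorite material.
; Its construction script creates a dynamic Meteorite material instance on the static mesh's first slot and registers it in the extract component's material group list.
; BeginPlay, inspector enter and exit, and extraction glow events only call the parent, which supplies the behavior.
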(event EventBeginPlay
  (|CallParentFunction))

(event EventItemExtractGlowing
  (params (bIsExtracting :type Boolean))
  (|CallParentFunction bIsExtracting))

(event EventEnterInspector
  (|CallParentFunction))

(event EventExitInspector
  (|CallParentFunction))

(fn ConstructionScript
  (|CallParentFunction)
  (bind _returnvalue (Rendering|Material|CreateDynamicMaterialInstance (Variables|Default|GetStaticMesh) 0 "/Game/Project/Artist/KeyObj/Material/Meteorite.Meteorite" "None" :!class /Script/Engine.PrimitiveComponent))
  (Utilities|Array|Add (Variables|/Game/Project/Core/InteractOBJ/AC_ExtractComponent.AC_ExtractComponent_C|GetExtractMatGroups (Variables|Default|GetAC_ExtractComponent)) _returnvalue))