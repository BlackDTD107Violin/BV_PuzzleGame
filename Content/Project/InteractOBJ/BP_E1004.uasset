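; BP_E1004 is an interactable object, apparently a sun coin given its SunCoin_Matal material, that supports inspection and item-extract glowing.
; Its events for begin play, inspector enter and exit, and extract glowing only forward to the parent class.
; The construction script creates a dynamic instance of that material on StaticMesh and adds it to the extract component's ExtractMatGroups.
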(event EventBeginPlay
  (|CallParentFunction))

(event EventEnterInspector
  (|CallParentFunction))

(event EventExitInspector
  (|CallParentFunction))

(event EventItemExtractGlowing
  (params (bIsExtracting :type Boolean))
  (|CallParentFunction bIsExtracting))

(fn ConstructionScript
  (|CallParentFunction)
  (bind _returnvalue (Rendering|Material|CreateDynamicMaterialInstance (Variables|Default|GetStaticMesh) 0 "/Game/Project/Artist/KeyObj/Material/SunCoin_Matal.SunCoin_Matal" "None" :!class /Script/Engine.PrimitiveComponent))
  (Utilities|Array|Add (Variables|/Game/Project/Core/InteractOBJ/AC_ExtractComponent.AC_ExtractComponent_C|GetExtractMatGroups (Variables|Default|GetAC_ExtractComponent)) _returnvalue))