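; Prototype interactable wheel that the player rotates by click-dragging, with configurable tint, inertia, whole-number snapping and allowed direction.
; Drag speed derives from the cursor's horizontal screen offset from the wheel's projected center, zeroed against the allowed direction.
; Free mode can coast with friction after release; whole-number mode matches the angle to equal divisions and lerps toward that step.
; Tick logic starts only after SetPivotWhenZoomIn's delayed setup measures mesh radius.
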(event OnEndCursorOver(WheelTA)
  (params (TouchedComponent :type Primitive%20Component%20Object%20Reference))
  (CallFunction|DragCanceling))

(event OnReleased(WheelTA)
  (params (TouchedComponent :type Primitive%20Component%20Object%20Reference) (ButtonReleased :type Key%20Structure :default "None"))
  (CallFunction|DragCanceling))

(event OnClicked(WheelTA)
  (params (TouchedComponent :type Primitive%20Component%20Object%20Reference) (ButtonPressed :type Key%20Structure :default "None"))
  (Variables|Default|SetbIsDragging true))

(event Custom|SetDemoMode
  (params (ColorType :type Integer) (bInertia :type Boolean) (bWholeNumber :type Boolean) (DirLimited :type E_DirLimited%20Enum :default "NewEnumerator0"))
  (Variables|Default|SetColorType ColorType)
  (Variables|Default|SetbHasInertia bInertia)
  (Variables|Default|SetbWholeNumber bWholeNumber)
  (Variables|Default|SetRotateDir DirLimited)
  (bind _returnvalue (Rendering|Material|CreateDynamicMaterialInstance (Variables|Default|GetWheel) 0 "/Game/Project/MaterialLibrary/DebugOrDemo/M_TestSolidColorInstance.M_TestSolidColorInstance" "" :!class /Script/Engine.PrimitiveComponent))
  (Rendering|Material|SetVectorParameterValue _returnvalue "Tint Color" (Math|Conversions|ToLinearColor(Color) (Utilities|Array|Get(acopy) (Variables|Default|GetColorArray) (Variables|Default|GetColorType))) :!class /Script/Engine.MaterialInstanceDynamic))

(event Custom|SetPivotWhenZoomIn
  (if (not (Variables|Default|GetbHaveSetViewportCenter))
    (Utilities|FlowControl|Delay 0.6)
    (Variables|Default|SetbHaveSetViewportCenter true)
    (Variables|Default|SetMeshRadius (.SphereRadius (Collision|GetComponentBounds (Variables|Default|GetWheel))))
    (if (Variables|Default|GetbWholeNumber)
      (bind _initangle (CallFunction|InitialRotateState))
      (bind _output_get (Variables|Default|SetCurrent%20Input _initangle))
      (CallFunction|AssignAngletoUnitsInitial _output_get)
      (CallFunction|WholeRotationFixed true))))

(event EventBeginPlay
  (bind _returnvalue (Game|GetPlayerController 0))
  (|CallParentFunction)
  (bind _asbp_first_person_character (Utilities|Casting|CastToBP_FirstPersonCharacter (Game|GetPlayerCharacter 0)))
  (Variables|Default|SetPlayer _asbp_first_person_character)
  (Input|EnableInput _returnvalue)
  (Variables|/Script/Engine.PlayerController|SetbEnableClickEvents _returnvalue true)
  (Variables|/Script/Engine.PlayerController|SetbEnableMouseOverEvents _returnvalue true))

(event EventTick
  (params (DeltaSeconds :type Float%20%28single-precision%29))
  (if (Variables|Default|GetbHaveSetViewportCenter)
    (if (Variables|Default|GetbWholeNumber)
      (if (Variables|Default|GetbIsDragging)
        (bind _currentinput (CallFunction|UpdatePlayerInput))
        (Variables|Default|SetCurrent%20Input _currentinput)
        (else
          (bind _bmatchdir (CallFunction|AssignAngletoUnits (Variables|Default|GetCurrent%20Input)))
          (CallFunction|WholeRotationFixed _bmatchdir)))
      (else
        (CallFunction|UpdateVelocity)
        (CallFunction|UpdateRotateMode)))))

(fn ConstructionScript
  (|CallParentFunction))

(fn UpdateRotateMode
  (if (Variables|Default|GetbIsDragging)
    (CallFunction|RotateViaPlayerInput)
    (elif (Variables|Default|GetbHasInertia)
      (CallFunction|RotateViaInertia))))

(fn UpdateVelocity
  (if (not (Variables|Default|GetbIsDragging))
    (if (and (< (Variables|Default|GetRotateVelocity) 0.1) (> (Variables|Default|GetRotateVelocity) -0.1))
      (Variables|Default|SetRotateVelocity 0.0)
      (else
        (Variables|Default|SetRotateVelocity (* (Variables|Default|GetRotateVelocity) (Variables|Default|GetFriction)))))))

(fn RotateViaPlayerInput
  (bind _returnvalue (Game|GetPlayerController 0))
  (Variables|Default|SetCurrentMousePivotX (.x (.ScreenLocation (Class|PlayerController|ProjectWorldLocationtoScreen _returnvalue (.WorldLocation (Game|Player|ConvertMouseLocationToWorldSpace _returnvalue)) false))))
  (if (Variables|Default|GetbReHandle)
    (Variables|Default|SetbReHandle false)
    (else
      (bind _returnvalue_2 (CallFunction|UpdateRotateVelocity))
      (Transformation|AddLocalRotation (Variables|Default|GetWheel) (Math|Rotator|MakeRotator 0.0 _returnvalue_2 0.0) false false))))

(fn RotateViaInertia
  (Transformation|AddLocalRotation (Variables|Default|GetWheel) (Math|Rotator|MakeRotator 0.0 (Variables|Default|GetRotateVelocity) 0.0) false false))

(fn InitialRotateState
  (Utilities|FlowControl|Sequence
    (:then_0
      (Variables|Default|SetAngleUnits (Math|Conversions|ToFloat(Integer) (/ 360 (Variables|Default|GetDividedCount)))))
    (:then_1
      (LocalVariables|SetHandlerInitPivot (Variables|/Script/Engine.SceneComponent|GetRelativeLocation (Variables|Default|GetHandler)))
      (LocalVariables|SetWheelInitPivot (Variables|/Script/Engine.SceneComponent|GetRelativeLocation (Variables|Default|GetWheel)))
      (if true
        (return (- 3.6e+02 (Class|KismetMathLibrary|DegAcos (Math|Vector|DotProduct (Math|Vector|Normalize (- (LocalVariables|GetHandlerInitPivot) (LocalVariables|GetWheelInitPivot))) (Math|Vector|Normalize (- (+ (LocalVariables|GetWheelInitPivot) "0.000000,-400.000000,0.000000") (LocalVariables|GetWheelInitPivot)))))))
        (else
          (return (- (Class|KismetMathLibrary|DegAcos (Math|Vector|DotProduct (Math|Vector|Normalize (- (LocalVariables|GetHandlerInitPivot) (LocalVariables|GetWheelInitPivot))) (Math|Vector|Normalize (- (+ (LocalVariables|GetWheelInitPivot) "0.000000,-400.000000,0.000000") (LocalVariables|GetWheelInitPivot))))) -9e+01)))))))

(fn DividedRangeLooping
  (params (DevidedCount :type Integer))
  (LocalVariables|SetTargetUnits (* (Variables|Default|GetAngleUnits) DevidedCount))
  (Utilities|FlowControl|Sequence
    (:then_0
      (Variables|Default|SetRangeMax (+ (LocalVariables|GetTargetUnits) (/ (Variables|Default|GetAngleUnits) 2.0))))
    (:then_1
      (Variables|Default|SetRangeMin (- (LocalVariables|GetTargetUnits) (/ (Variables|Default|GetAngleUnits) 2.0))))
    (:then_2
      (if (> (Variables|Default|GetRangeMax) 3.6e+02)
        (Variables|Default|SetRangeMax (- (Variables|Default|GetRangeMax) 3.6e+02))
        (Variables|Default|SetbCrossZero true))
      (if (< (Variables|Default|GetRangeMin) 0.0)
        (Variables|Default|SetRangeMin (+ (Variables|Default|GetRangeMin) 3.6e+02))
        (Variables|Default|SetbCrossZero true)
        (return (LocalVariables|GetTargetUnits))
        (else
          (Variables|Default|SetbCrossZero false)
          (return (LocalVariables|GetTargetUnits)))))))

(fn CheckAngleRange
  (params (TargetUnits :type Float%20%28double-precision%29) (InputAngle :type Float%20%28double-precision%29))
  (Variables|Default|SetCurrentUnits (* TargetUnits -1.0))
  (LocalVariables|SetInput InputAngle)
  (if (Variables|Default|GetbCrossZero)
    (if (> (- (LocalVariables|GetInput) 1.8e+02) 0.0)
      (if (and (> (LocalVariables|GetInput) (Variables|Default|GetRangeMin)) (<= (LocalVariables|GetInput) (+ (Variables|Default|GetRangeMax) 3.6e+02)))
        (Variables|Default|SetLatestUnits (Variables|Default|GetCurrentUnits))
        (return true)
        (else
          (return false)))
      (elif (and (> (LocalVariables|GetInput) (- (Variables|Default|GetRangeMin) 3.6e+02)) (<= (LocalVariables|GetInput) (Variables|Default|GetRangeMax)))
        (Variables|Default|SetLatestUnits (Variables|Default|GetCurrentUnits))
        (return true)
        (else
          (return false))))
    (elif (and (> (LocalVariables|GetInput) (Variables|Default|GetRangeMin)) (<= (LocalVariables|GetInput) (Variables|Default|GetRangeMax)))
      (Variables|Default|SetLatestUnits (Variables|Default|GetCurrentUnits))
      (return true)
      (else
        (return false)))))

(fn UpdatePlayerInput
  (bind _returnvalue (Game|GetPlayerController 0))
  (Variables|Default|SetCurrentMousePivotX (.x (.ScreenLocation (Class|PlayerController|ProjectWorldLocationtoScreen _returnvalue (.WorldLocation (Game|Player|ConvertMouseLocationToWorldSpace _returnvalue)) false))))
  (if (Variables|Default|GetbReHandle)
    (Variables|Default|SetbReHandle false)
    (else
      (bind _returnvalue_2 (CallFunction|UpdateRotateVelocityWholeNumber))
      (Transformation|AddLocalRotation (Variables|Default|GetWheel) (Math|Rotator|MakeRotator 0.0 _returnvalue_2 0.0) false false)
      (return (Class|KismetMathLibrary|ClampAxis (* (.yaw (Variables|/Script/Engine.SceneComponent|GetRelativeRotation (Variables|Default|GetWheel))) -1.0))))))

(fn UpdateRotateVelocity
  (bind _wheel (Variables|Default|GetWheel))
  (bind _relativelocation (Variables|/Script/Engine.SceneComponent|GetRelativeLocation _wheel))
  (Utilities|FlowControl|Sequence
    (:then_0
      (Variables|Default|SetRotateVelocity (* (/ (- (Variables|Default|GetCurrentMousePivotX) (.x (.ScreenPosition (Class|GameplayStatics|ProjectWorldtoScreen (Game|GetPlayerController 0) (Variables|/Script/Engine.SceneComponent|GetRelativeLocation (Variables|Default|GetWheel)) false)))) (.x (.ScreenPosition (Class|GameplayStatics|ProjectWorldtoScreen (Game|GetPlayerController 0) (Math|Vector|MakeVector (+ (.x _relativelocation) (Variables|Default|GetMeshRadius)) (.y _relativelocation) (.z _relativelocation)) false)))) 2.5)))
    (:then_1
      (switch Utilities|FlowControl|Switch|SwitchonE_DirLimited (Variables|Default|GetRotateDir)
        (:NewEnumerator0
          _)
        (:NewEnumerator1
          (if (> (Variables|Default|GetRotateVelocity) 0.0)
            _
            (else
              (bind _output_get (Variables|Default|SetRotateVelocity 0.0 :!label _label))
              (return _output_get))))
        (:NewEnumerator2
          (if (< (Variables|Default|GetRotateVelocity) 0.0)
            _
            (else
              (goto _label)))))
      (return (Variables|Default|GetRotateVelocity)))))

(fn AssignAngletoUnits
  (params (InputAngle :type Float%20%28double-precision%29))
  (Variables|Default|SetCurrentACOSdResult InputAngle)
  (if (Variables|Default|GetbContinueRotate)
    (bind _index (Utilities|FlowControl|ForLoopwithBreak 0 (- (Variables|Default|GetDividedCount) 1) :!label _label)
      (:LoopBody
        (bind _output_get (LocalVariables|SetCurrentMatchIndex _index))
        (bind _targetunit (CallFunction|DividedRangeLooping _output_get))
        (bind _bfound (CallFunction|CheckAngleRange _targetunit (Variables|Default|GetCurrentACOSdResult)))
        (if _bfound
          (goto _label Break)))
      (:Completed
        (switch Utilities|FlowControl|Switch|SwitchonE_DirLimited (Variables|Default|GetRotateDir)
          (:NewEnumerator0
            (Variables|Default|SetLatestMatchIndex (LocalVariables|GetCurrentMatchIndex))
            (Variables|Default|SetLatestACOSdResult (Variables|Default|GetCurrentACOSdResult))
            (return true))
          (:NewEnumerator1
            (CallFunction|CheckPositiveInput (LocalVariables|GetCurrentMatchIndex))
            (return true))
          (:NewEnumerator2
            (CallFunction|CheckNegativeInput (LocalVariables|GetCurrentMatchIndex))
            (return true)))))))

(fn WholeRotationFixed
  (params (bMatchDir :type Boolean))
  (bind _wheel (Variables|Default|GetWheel))
  (bind _relativerotation (Variables|/Script/Engine.SceneComponent|GetRelativeRotation _wheel))
  (if bMatchDir
    (Transformation|SetRelativeRotation (Variables|Default|GetWheel) (Math|Rotator|Lerp(Rotator) (Variables|/Script/Engine.SceneComponent|GetRelativeRotation (Variables|Default|GetWheel)) (Math|Rotator|MakeRotator (.roll _relativerotation) (.pitch _relativerotation) (Variables|Default|GetCurrentUnits)) 0.1 true) false false)))

(fn GetAngleCurrent&MainMesh
  (Utilities|FlowControl|Sequence
    (:then_0
      (bind _returnvalue (CallFunction|GetAngleCurrent&LatestWholeNumVer))
      (LocalVariables|SetDotResult _returnvalue))
    (:then_1
      (bind (_crossvectory _acosd) (CallFunction|GetAngleCurrent&MainMeshWholeNumVer))
      (return _crossvectory _acosd true))))

(fn GetAngleCurrent&LatestWholeNumVer
  (return (Class|KismetMathLibrary|CrossProduct2D (Math|Vector2D|Normalize2D (- (Variables|Default|GetCurrentMousePivot) (Variables|Default|GetViewportCenter))) (Math|Vector2D|Normalize2D (- (+ (Variables|Default|GetViewportCenter) "(X=0.000000,Y=-400.000000)") (Variables|Default|GetViewportCenter))))))

(fn GetAngleCurrent&MainMeshWholeNumVer
  (bind _currentmousepivot (Variables|Default|GetCurrentMousePivot))
  (bind _viewportcenter (Variables|Default|GetViewportCenter))
  (bind _viewportcenter_2 (Variables|Default|GetViewportCenter))
  (bind _viewportcenter_3 (Variables|Default|GetViewportCenter))
  (bind _returnvalue (+ _viewportcenter_2 "(X=0.000000,Y=-400.000000)"))
  (bind _returnvalue_2 (- _currentmousepivot _viewportcenter))
  (bind _returnvalue_3 (Math|Vector2D|Normalize2D _returnvalue_2))
  (bind _returnvalue_4 (- _returnvalue _viewportcenter_3))
  (bind _returnvalue_5 (Math|Vector2D|Normalize2D _returnvalue_4))
  (return (Class|KismetMathLibrary|CrossProduct2D _returnvalue_3 _returnvalue_5) (Class|KismetMathLibrary|DegAcos (Math|Vector2D|DotProduct(2D) _returnvalue_3 _returnvalue_5))))

(fn DragCanceling
  (Variables|Default|SetbReHandle true)
  (if (and (Variables|Default|GetbWholeNumber) (Variables|Default|GetbIsDragging))
    (CallFunction|WholeRotationFixed (Variables|Default|GetbMatchDir)))
  (Variables|Default|SetbIsDragging false)
  (Variables|Default|SetbDragValueIsValid false))

(fn AssignAngletoUnitsInitial
  (params (InputAngle :type Float%20%28double-precision%29))
  (Variables|Default|SetLatestACOSdResult InputAngle)
  (if (and (Variables|Default|GetbContinueRotate) (Variables|Default|GetbMatchDir))
    (bind _index (Utilities|FlowControl|ForLoopwithBreak 0 (- (Variables|Default|GetDividedCount) 1) :!label _label)
      (:LoopBody
        (bind _output_get (Variables|Default|SetLatestMatchIndex _index))
        (bind _targetunit (CallFunction|DividedRangeLooping _output_get))
        (bind _bfound (CallFunction|CheckAngleRange _targetunit (Variables|Default|GetLatestACOSdResult)))
        (if _bfound
          (goto _label Break))))))

(fn CheckPositiveInput
  (params (CurrentMatchIndex :type Integer))
  (LocalVariables|SetCurrent CurrentMatchIndex)
  (Variables|Default|SetbMatchDir false)
  (Utilities|FlowControl|Sequence
    (:then_0
      (LocalVariables|SetIndexGap (- (LocalVariables|GetCurrent) (Variables|Default|GetLatestMatchIndex)))
      (LocalVariables|SetACOsdGap (- (Variables|Default|GetCurrentACOSdResult) (Variables|Default|GetLatestACOSdResult))))
    (:then_1
      (if (> (LocalVariables|GetIndexGap) 0)
        (LocalVariables|SetbMatch&Update true)
        (elif (== (LocalVariables|GetIndexGap) 0)
          (if (or (> (LocalVariables|GetACOsdGap) 0.0) (and (== (LocalVariables|GetACOsdGap) 0.0) (Variables|Default|GetbDragValueIsValid)))
            (Variables|Default|SetbDragValueIsValid true)
            (LocalVariables|SetbMatch&Update true)
            (else
              (LocalVariables|SetbMatch&Update false)
              (if (< (LocalVariables|GetACOsdGap) 0.0)
                (Variables|Default|SetLatestACOSdResult (Variables|Default|GetCurrentACOSdResult)))))
          (elif (== (* (LocalVariables|GetIndexGap) -1) (- (Variables|Default|GetDividedCount) 1))
            (LocalVariables|SetbMatch&Update true)
            (else
              (LocalVariables|SetbMatch&Update false))))))
    (:then_2
      (if (LocalVariables|GetbMatch&Update)
        (Variables|Default|SetLatestMatchIndex (LocalVariables|GetCurrent))
        (Variables|Default|SetLatestACOSdResult (Variables|Default|GetCurrentACOSdResult))
        (return true)
        (else
          (return false))))))

(fn CheckNegativeInput
  (params (CurrentMatchIndex :type Integer))
  (LocalVariables|SetCurrent CurrentMatchIndex)
  (Variables|Default|SetbMatchDir false)
  (Utilities|FlowControl|Sequence
    (:then_0
      (LocalVariables|SetIndexGap (- (LocalVariables|GetCurrent) (Variables|Default|GetLatestMatchIndex)))
      (LocalVariables|SetACOsdGap (- (Variables|Default|GetCurrentACOSdResult) (Variables|Default|GetLatestACOSdResult))))
    (:then_1
      (if (< (LocalVariables|GetIndexGap) 0)
        (LocalVariables|SetbMatch&Update true)
        (elif (== (LocalVariables|GetIndexGap) 0)
          (if (or (< (LocalVariables|GetACOsdGap) 0.0) (and (== (LocalVariables|GetACOsdGap) 0.0) (Variables|Default|GetbDragValueIsValid)))
            (Variables|Default|SetbDragValueIsValid true)
            (LocalVariables|SetbMatch&Update true)
            (else
              (LocalVariables|SetbMatch&Update false)
              (if (> (LocalVariables|GetACOsdGap) 0.0)
                (Variables|Default|SetLatestACOSdResult (Variables|Default|GetCurrentACOSdResult)))))
          (elif (== (LocalVariables|GetIndexGap) (- (Variables|Default|GetDividedCount) 1))
            (LocalVariables|SetbMatch&Update true)
            (else
              (LocalVariables|SetbMatch&Update false))))))
    (:then_2
      (if (LocalVariables|GetbMatch&Update)
        (Variables|Default|SetLatestMatchIndex (LocalVariables|GetCurrent))
        (Variables|Default|SetLatestACOSdResult (Variables|Default|GetCurrentACOSdResult))
        (return true)
        (else
          (return false))))))

(fn UpdateRotateVelocityWholeNumber
  (bind _wheel (Variables|Default|GetWheel))
  (bind _relativelocation (Variables|/Script/Engine.SceneComponent|GetRelativeLocation _wheel))
  (Utilities|FlowControl|Sequence
    (:then_0
      (Variables|Default|SetRotateVelocity (* (/ (- (Variables|Default|GetCurrentMousePivotX) (.x (.ScreenPosition (Class|GameplayStatics|ProjectWorldtoScreen (Game|GetPlayerController 0) (Variables|/Script/Engine.SceneComponent|GetRelativeLocation (Variables|Default|GetWheel)) false)))) (.x (.ScreenPosition (Class|GameplayStatics|ProjectWorldtoScreen (Game|GetPlayerController 0) (Math|Vector|MakeVector (+ (.x _relativelocation) (Variables|Default|GetMeshRadius)) (.y _relativelocation) (.z _relativelocation)) false)))) 2.5)))
    (:then_1
      (switch Utilities|FlowControl|Switch|SwitchonE_DirLimited (Variables|Default|GetRotateDir)
        (:NewEnumerator0
          _)
        (:NewEnumerator1
          (if (> (Variables|Default|GetRotateVelocity) 0.0)
            _
            (else
              (bind _output_get (Variables|Default|SetRotateVelocity 0.0 :!label _label))
              (return _output_get))))
        (:NewEnumerator2
          (if (< (Variables|Default|GetRotateVelocity) 0.0)
            _
            (else
              (goto _label)))))
      (return (Variables|Default|GetRotateVelocity)))))