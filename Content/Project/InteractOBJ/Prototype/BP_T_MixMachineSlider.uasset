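; Interactable slider prop for the mix and extract machines, with a zoom-in view for the player.
; Zooming blends the camera to this actor, locks move and look input and swaps mesh collision; zooming out restores them.
; A matching code clears the lock, and ending interaction cancels the child slider's drag.
; Assign functions pass the machine reference to the child slider bar, flagging extract machine use.
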(event EventBeginPlay
  (|CallParentFunction)
  (bind _asbp_first_person_character (Utilities|Casting|CastToBP_FirstPersonCharacter (Game|GetPlayerCharacter 0)))
  (Variables|Default|SetPlayer _asbp_first_person_character))

(event EventInteractEnd
  (bind _asbp_s0003 (Utilities|Casting|CastToBP_S0003 (Variables|/Script/Engine.ChildActorComponent|GetChildActor (Variables|Default|GetSlider))))
  (Default|CancelingDrag _asbp_s0003))

(event EventZoomin
  (params (ZoomComponent :type Actor%20Component%20Object%20Reference))
  (bind _returnvalue (Game|GetPlayerController 0))
  (Game|Player|SetViewTargetwithBlend (Game|GetPlayerController 0) self 0.5 "VTBlend_Linear" 0.0 true)
  (Input|SetIgnoreMoveInput _returnvalue true)
  (Input|SetIgnoreLookInput _returnvalue true)
  (Default|ClearGamePromptUIView (Variables|Default|GetPlayer))
  (Collision|SetCollisionProfileName (Variables|Default|GetStaticMesh) "TRICKignore" true :!class /Script/Engine.PrimitiveComponent))

(event EventZoomOut
  (bind _returnvalue (Game|GetPlayerController 0))
  (Game|Player|SetViewTargetwithBlend (Game|GetPlayerController 0) (Game|GetPlayerCharacter 0) 0.5 "VTBlend_Linear" 0.0 true)
  (Input|ResetIgnoreMoveInput _returnvalue)
  (Input|ResetIgnoreLookInput _returnvalue)
  (Utilities|FlowControl|Delay 0.5)
  (Collision|SetCollisionProfileName (Variables|Default|GetStaticMesh) "BlockAllDynamic" true :!class /Script/Engine.PrimitiveComponent))

(event EventInteractiveUnlocked
  (params (AttachKEY :type Actor%20Object%20Reference) (MatchOBJCode :type Name :default "None"))
  (Utilities|FlowControl|Delay 0.2)
  (if (Utilities|Enum|Equal(Enum) (Utilities|String|ToString(Name) MatchOBJCode) (Utilities|String|ToString(Name) (Variables|Default|GetSETMatchCode)))
    (Variables|Default|SetbIsLocked false)))

(fn ConstructionScript
  (|CallParentFunction))

(fn AssignMixMachinetoChild
  (params (REF%20GlassMixMachine :type BP%20Glass%20Mix%20Machine%20Object%20Reference))
  (bind _asbp_mix_machine_slider_bar (Utilities|Casting|CastToBP_MixMachineSliderBar (Variables|/Script/Engine.ChildActorComponent|GetChildActor (Variables|Default|GetSlider))))
  (Variables|/Game/Project/InteractOBJ/Prototype/BP_MixMachineSliderBar.BP_MixMachineSliderBar_C|SetREF_GlassMixMachine _asbp_mix_machine_slider_bar REF%20GlassMixMachine))

(fn AssignExtractMachinetoChild
  (params (REF%20ExtractMachine :type BP%20Extract%20Machine%20Object%20Reference))
  (bind _asbp_mix_machine_slider_bar (Utilities|Casting|CastToBP_MixMachineSliderBar (Variables|/Script/Engine.ChildActorComponent|GetChildActor (Variables|Default|GetSlider))))
  (Variables|/Game/Project/InteractOBJ/Prototype/BP_MixMachineSliderBar.BP_MixMachineSliderBar_C|SetREF_ExtractMachine _asbp_mix_machine_slider_bar REF%20ExtractMachine)
  (Variables|/Game/Project/InteractOBJ/Prototype/BP_MixMachineSliderBar.BP_MixMachineSliderBar_C|SetbIsExtractMachine _asbp_mix_machine_slider_bar true))