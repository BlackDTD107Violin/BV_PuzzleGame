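; BP_T0002 is a prototype tutorial interactable that the first-person player can zoom into and out of.
; Zooming blends the view to this actor and back, toggling player move/look input and the mesh's collision profile.
; The first zoom-in, and the first zoom-out after taking an item, each trigger a player tutorial step.
; A matching code clears its lock, and ending interaction cancels dragging on the LearnBox child BP_S0003.
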(event EventBeginPlay
  (|CallParentFunction)
  (bind _asbp_first_person_character_tutorial (Utilities|Casting|CastToBP_FirstPersonCharacterTutorial (Game|GetPlayerCharacter 0)))
  (Variables|Default|SetPlayer _asbp_first_person_character_tutorial))

(event EventInteractEnd
  (bind _asbp_s0003 (Utilities|Casting|CastToBP_S0003 (Variables|/Script/Engine.ChildActorComponent|GetChildActor (Variables|Default|GetLearnBox))))
  (Default|CancelingDrag _asbp_s0003))

(event EventZoomin
  (params (ZoomComponent :type Actor%20Component%20Object%20Reference))
  (bind _returnvalue (Game|GetPlayerController 0))
  (bind _player (Variables|Default|GetPlayer))
  (Utilities|FlowControl|Sequence
    (:then_0
      (Game|Player|SetViewTargetwithBlend (Game|GetPlayerController 0) self 0.5 "VTBlend_Linear" 0.0 true)
      (Input|SetIgnoreMoveInput _returnvalue true)
      (Input|SetIgnoreLookInput _returnvalue true)
      (Default|ClearGamePromptUIView (Variables|Default|GetPlayer))
      (Collision|SetCollisionProfileName (Variables|Default|GetStaticMesh) "TRICKignore" true :!class /Script/Engine.PrimitiveComponent))
    (:then_1
      (if (not (Variables|Default|GetbHasTriggerTutor))
        (Variables|Default|SetbHasTriggerTutor true)
        (Utilities|FlowControl|Delay 0.5)
        (Default|ArriveTutorialTA _player)
        (Default|ClearGamePromptUIView _player)))))

(event EventZoomOut
  (bind _returnvalue (Game|GetPlayerController 0))
  (Utilities|FlowControl|Sequence
    (:then_0
      (Game|Player|SetViewTargetwithBlend (Game|GetPlayerController 0) (Game|GetPlayerCharacter 0) 0.5 "VTBlend_Linear" 0.0 true)
      (Input|ResetIgnoreMoveInput _returnvalue)
      (Input|ResetIgnoreLookInput _returnvalue)
      (Utilities|FlowControl|Delay 0.5)
      (Collision|SetCollisionProfileName (Variables|Default|GetStaticMesh) "BlockAllDynamic" true :!class /Script/Engine.PrimitiveComponent))
    (:then_1
      (if (and (not (Variables|Default|GetbItemTutorHasTrigger)) (Variables|Default|GetbHasTakeItem))
        (Variables|Default|SetbItemTutorHasTrigger true)
        (Default|ArriveTutorialTA (Variables|Default|GetPlayer))))))

(event EventInteractiveUnlocked
  (params (AttachKEY :type Actor%20Object%20Reference) (MatchOBJCode :type Name :default "None"))
  (Utilities|FlowControl|Delay 0.2)
  (if (Utilities|Enum|Equal(Enum) (Utilities|String|ToString(Name) MatchOBJCode) (Utilities|String|ToString(Name) (Variables|Default|GetSETMatchCode)))
    (Variables|Default|SetbIsLocked false)))

(fn ConstructionScript
  (|CallParentFunction))