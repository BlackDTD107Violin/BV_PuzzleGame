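; Prototype mouse-dragged rotary wheel inside BP_CollectionMachineDemo_beta that selects one of DividedCount notches for the inserted GLASS code.
; While dragging, the cursor's screen-space angle around the projected pivot, via dot and cross products, maps to a notch index and updates the parent machine.
; Tick eases the wheel toward that notch with a shortest-path lerp.
; Free-spin inertia and positive-direction check functions exist but are not called here.
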(event OnBeginCursorOver(Handler)
  (params (TouchedComponent :type Primitive%20Component%20Object%20Reference))
  (Variables|Default|SetbContinueRotate true)
  (Variables|Default|SetbStillInHandler true))

(event OnEndCursorOver(Handler)
  (params (TouchedComponent :type Primitive%20Component%20Object%20Reference))
  (Utilities|FlowControl|Delay 0.01)
  (Variables|Default|SetbStillInHandler false)
  (if (not (Variables|Default|GetbStillInWheel))
    (CallFunction|DragCanceling)))

(event OnClicked(Handler)
  (params (TouchedComponent :type Primitive%20Component%20Object%20Reference) (ButtonPressed :type Key%20Structure))
  (Variables|Default|SetbIsDragging true))

(event OnReleased(Handler)
  (params (TouchedComponent :type Primitive%20Component%20Object%20Reference) (ButtonReleased :type Key%20Structure))
  (CallFunction|DragCanceling))

(event OnBeginCursorOver(WheelTA)
  (params (TouchedComponent :type Primitive%20Component%20Object%20Reference))
  (Variables|Default|SetbStillInWheel true))

(event OnEndCursorOver(WheelTA)
  (params (TouchedComponent :type Primitive%20Component%20Object%20Reference))
  (Utilities|FlowControl|Delay 0.01)
  (if (not (Variables|Default|GetbStillInHandler))
    (CallFunction|DragCanceling)))

(event OnReleased(WheelTA)
  (params (TouchedComponent :type Primitive%20Component%20Object%20Reference) (ButtonReleased :type Key%20Structure))
  (CallFunction|DragCanceling)
  (Variables|Default|SetbStillInWheel false))

(event Custom|SetPivotWhenZoomIn
  (if (not (Variables|Default|GetbHaveSetViewportCenter))
    (Utilities|FlowControl|Delay 0.6)
    (Variables|Default|SetbHaveSetViewportCenter true)
    (Variables|Default|SetViewportCenter (.ScreenPosition (Class|GameplayStatics|ProjectWorldtoScreen (Game|GetPlayerController 0) (Variables|/Script/Engine.SceneComponent|GetRelativeLocation (Variables|Default|GetWheel)) false)))
    (bind _initangle (CallFunction|InitialRotateState))
    (CallFunction|AssignAngletoUnitsInitial _initangle)
    (CallFunction|WholeRotationFixed true)))

(event EventBeginPlay
  (bind _returnvalue (Game|GetPlayerController 0))
  (|CallParentFunction)
  (bind _asbp_first_person_character (Utilities|Casting|CastToBP_FirstPersonCharacter (Game|GetPlayerCharacter 0)))
  (Variables|Default|SetPlayer _asbp_first_person_character)
  (Input|EnableInput _returnvalue)
  (Variables|/Script/Engine.PlayerController|SetbEnableClickEvents _returnvalue true)
  (Variables|/Script/Engine.PlayerController|SetbEnableMouseOverEvents _returnvalue true)
  (bind _returnvalue_2 (Rendering|Material|CreateDynamicMaterialInstance (Variables|Default|GetWheel) 0 "/Game/Project/MaterialLibrary/DebugOrDemo/M_TestSolidColorInstance.M_TestSolidColorInstance" "" :!class /Script/Engine.PrimitiveComponent))
  (Rendering|Material|SetVectorParameterValue _returnvalue_2 "Tint Color" (Variables|Default|GetMachineColor) :!class /Script/Engine.MaterialInstanceDynamic)
  (bind _asbp_collection_machine_demo_beta (Utilities|Casting|CastToBP_CollectionMachineDemo_beta (Actor|GetParentActor)))
  (Variables|Default|SetREF_Collection%20Machine%20Demo%20Beta _asbp_collection_machine_demo_beta))

(event EventTick
  (params (DeltaSeconds :type Float%20%28single-precision%29))
  (if (Variables|Default|GetbHaveSetViewportCenter)
    (if (Variables|Default|GetbHasInsertedGLASS)
      (if (Variables|Default|GetbIsDragging)
        (bind _currentinput (CallFunction|UpdatePlayerInput))
        (bind _bmatchdir (CallFunction|AssignAngletoUnits _currentinput))
        (bind _output_get (Variables|Default|SetbMatchDir _bmatchdir))
        (CallFunction|WholeRotationFixed _output_get)
        (else
          (CallFunction|WholeRotationFixed (Variables|Default|GetbMatchDir) :!label _label)))
      (else
        (goto _label)))))

(fn ConstructionScript
  (|CallParentFunction))

(fn UpdateRotateMode
  (if (Variables|Default|GetbIsDragging)
    (CallFunction|RotateViaPlayerInput)
    (elif (Variables|Default|GetbHasInertia)
      (CallFunction|RotateViaInertia))))

(fn UpdateVelocity
  (if (Variables|Default|GetbIsDragging)
    (Variables|Default|SetRotateVelocity 6e+01)
    (elif (< (Variables|Default|GetRotateVelocity) 0.1)
      (Variables|Default|SetRotateVelocity 0.0)
      (else
        (Variables|Default|SetRotateVelocity (* (Variables|Default|GetRotateVelocity) (Variables|Default|GetFriction)))))))

(fn RotateViaPlayerInput
  (bind _returnvalue (Game|GetPlayerController 0))
  (bind _returnvalue_2 (Game|GetPlayerController 0))
  (bind _worldlocation (Game|Player|ConvertMouseLocationToWorldSpace _returnvalue))
  (Variables|Default|SetCurrentMouseVector (Math|Vector|MakeVector (.x _worldlocation) (.y (Variables|/Script/Engine.SceneComponent|GetRelativeLocation (Variables|Default|GetWheel))) (.z _worldlocation)))
  (Variables|Default|SetCurrentMousePivot (.ScreenLocation (Class|PlayerController|ProjectWorldLocationtoScreen _returnvalue_2 (.WorldLocation (Game|Player|ConvertMouseLocationToWorldSpace _returnvalue_2)) false)))
  (if (Variables|Default|GetbReHandle)
    (Variables|Default|SetbReHandle false)
    (else
      (bind _returnvalue_3 (CallFunction|GetAngleCurrent&Latest))
      (Variables|Default|SetLatestDotValue _returnvalue_3)
      (Transformation|AddLocalRotation (Variables|Default|GetWheel) (Math|Rotator|MakeRotator 0.0 (.pitch (Math|Rotator|MakeRotator 0.0 (* _returnvalue_3 (Variables|Default|GetRotateVelocity)) 0.0)) 0.0) false false)))
  (Variables|Default|SetLatestMouseVector (Variables|Default|GetCurrentMouseVector))
  (Variables|Default|SetLatestMousePivot (Variables|Default|GetCurrentMousePivot)))

(fn RotateViaInertia
  (Transformation|AddLocalRotation (Variables|Default|GetWheel) (Math|Rotator|MakeRotator 0.0 (.pitch (Math|Rotator|MakeRotator 0.0 (* (Variables|Default|GetLatestDotValue) (Variables|Default|GetRotateVelocity)) 0.0)) 0.0) false false))

(fn InitialRotateState
  (bind _viewportcenter (Variables|Default|GetViewportCenter))
  (bind _viewportcenter_2 (Variables|Default|GetViewportCenter))
  (bind _returnvalue (+ _viewportcenter "(X=0.000000,Y=-400.000000)"))
  (bind _returnvalue_2 (- _returnvalue _viewportcenter_2))
  (bind _returnvalue_3 (Math|Vector2D|Normalize2D _returnvalue_2))
  (Utilities|FlowControl|Sequence
    (:then_0
      (Variables|Default|SetAngleUnits (Math|Conversions|ToFloat(Integer) (/ 360 (Variables|Default|GetDividedCount)))))
    (:then_1
      (Variables|Default|SetCurrentMousePivot (.ScreenPosition (Class|GameplayStatics|ProjectWorldtoScreen (Game|GetPlayerController 0) (Variables|/Script/Engine.SceneComponent|GetRelativeLocation (Variables|Default|GetHandler)) false)))
      (if (> (Class|KismetMathLibrary|CrossProduct2D (Math|Vector2D|Normalize2D (- (Variables|Default|GetCurrentMousePivot) (Variables|Default|GetViewportCenter))) _returnvalue_3) 0.0)
        (return (- 3.6e+02 (Class|KismetMathLibrary|DegAcos (Math|Vector2D|DotProduct(2D) (Math|Vector2D|Normalize2D (- (Variables|Default|GetCurrentMousePivot) (Variables|Default|GetViewportCenter))) _returnvalue_3))))
        (else
          (return (- (Class|KismetMathLibrary|DegAcos (Math|Vector2D|DotProduct(2D) (Math|Vector2D|Normalize2D (- (Variables|Default|GetCurrentMousePivot) (Variables|Default|GetViewportCenter))) _returnvalue_3)) -9e+01)))))))

(fn DividedRangeLooping
  (params (DevidedCount :type Integer))
  (LocalVariables|SetTargetUnits (* (Variables|Default|GetAngleUnits) DevidedCount))
  (Utilities|FlowControl|Sequence
    (:then_0
      (Variables|Default|SetRangeMax (+ (LocalVariables|GetTargetUnits) (/ (Variables|Default|GetAngleUnits) 2.0))))
    (:then_1
      (Variables|Default|SetRangeMin (- (LocalVariables|GetTargetUnits) (/ (Variables|Default|GetAngleUnits) 2.0))))
    (:then_2
      (if (> (Variables|Default|GetRangeMax) 3.6e+02)
        (Variables|Default|SetRangeMax (- (Variables|Default|GetRangeMax) 3.6e+02))
        (Variables|Default|SetbCrossZero true))
      (if (< (Variables|Default|GetRangeMin) 0.0)
        (Variables|Default|SetRangeMin (+ (Variables|Default|GetRangeMin) 3.6e+02))
        (Variables|Default|SetbCrossZero true)
        (return (LocalVariables|GetTargetUnits))
        (else
          (Variables|Default|SetbCrossZero false)
          (return (LocalVariables|GetTargetUnits)))))))

(fn CheckAngleRange
  (params (TargetUnits :type Float%20%28double-precision%29) (InputAngle :type Float%20%28double-precision%29))
  (Variables|Default|SetCurrentUnits (* TargetUnits -1.0))
  (LocalVariables|SetInput InputAngle)
  (if (Variables|Default|GetbCrossZero)
    (if (> (- (LocalVariables|GetInput) 1.8e+02) 0.0)
      (if (and (> (LocalVariables|GetInput) (Variables|Default|GetRangeMin)) (<= (LocalVariables|GetInput) (+ (Variables|Default|GetRangeMax) 3.6e+02)))
        (Variables|Default|SetLatestUnits (Variables|Default|GetCurrentUnits))
        (return true)
        (else
          (return false)))
      (elif (and (> (LocalVariables|GetInput) (- (Variables|Default|GetRangeMin) 3.6e+02)) (<= (LocalVariables|GetInput) (Variables|Default|GetRangeMax)))
        (Variables|Default|SetLatestUnits (Variables|Default|GetCurrentUnits))
        (return true)
        (else
          (return false))))
    (elif (and (> (LocalVariables|GetInput) (Variables|Default|GetRangeMin)) (<= (LocalVariables|GetInput) (Variables|Default|GetRangeMax)))
      (Variables|Default|SetLatestUnits (Variables|Default|GetCurrentUnits))
      (return true)
      (else
        (return false)))))

(fn UpdatePlayerInput
  (bind _returnvalue (Game|GetPlayerController 0))
  (Variables|Default|SetCurrentMousePivot (.ScreenLocation (Class|PlayerController|ProjectWorldLocationtoScreen _returnvalue (.WorldLocation (Game|Player|ConvertMouseLocationToWorldSpace _returnvalue)) false)))
  (if (not (Utilities|Operators|EqualEqual (Variables|Default|GetCurrentMousePivot) (Variables|Default|GetLatestMousePivot) 0.0001))
    (bind (_crossresult _acosdresult _bmatchdir) (CallFunction|GetAngleCurrent&MainMesh))
    (bind _output_get (Variables|Default|SetbMatchDir _bmatchdir))
    (if (or _output_get (Variables|Default|GetbReHandle))
      _
      (else
        (Variables|Default|SetbContinueRotate false)))
    (if (Variables|Default|GetbReHandle)
      (Variables|Default|SetbReHandle false)
      (Variables|Default|SetLatestMousePivot (Variables|Default|GetCurrentMousePivot))
      (return (Variables|Default|GetLatestACOSdResult))
      (elif (> _crossresult 0.0)
        (return (- 3.6e+02 _acosdresult))
        (else
          (return _acosdresult))))))

(fn GetAngleCurrent&Latest
  (LocalVariables|SetDotResult (Class|KismetMathLibrary|CrossProduct2D (Math|Vector2D|Normalize2D (- (Variables|Default|GetCurrentMousePivot) (Variables|Default|GetViewportCenter))) (Math|Vector2D|Normalize2D (- (Variables|Default|GetLatestMousePivot) (Variables|Default|GetViewportCenter)))))
  (return (LocalVariables|GetDotResult)))

(fn AssignAngletoUnits
  (params (InputAngle :type Float%20%28double-precision%29))
  (Variables|Default|SetCurrentACOSdResult InputAngle)
  (if (Variables|Default|GetbContinueRotate)
    (bind _index (Utilities|FlowControl|ForLoopwithBreak 0 (- (Variables|Default|GetDividedCount) 1) :!label _label)
      (:LoopBody
        (bind _output_get (LocalVariables|SetCurrentMatchIndex _index))
        (bind _targetunit (CallFunction|DividedRangeLooping _output_get))
        (bind _bfound (CallFunction|CheckAngleRange _targetunit (Variables|Default|GetCurrentACOSdResult)))
        (if _bfound
          (goto _label Break)))
      (:Completed
        (Variables|Default|SetLatestMatchIndex (LocalVariables|GetCurrentMatchIndex))
        (Variables|Default|SetInsertedGLASSUnits (LocalVariables|GetCurrentMatchIndex))
        (Default|UpdateGLASSCodefromEachFunc (Variables|Default|GetREF_Collection%20Machine%20Demo%20Beta))
        (Variables|Default|SetLatestACOSdResult (Variables|Default|GetCurrentACOSdResult))
        (Variables|Default|SetLatestMousePivot (Variables|Default|GetCurrentMousePivot))
        (return true)))))

(fn WholeRotationFixed
  (params (bMatchDir :type Boolean))
  (if bMatchDir
    (Transformation|SetRelativeRotation (Variables|Default|GetWheel) (Math|Rotator|Lerp(Rotator) (Variables|/Script/Engine.SceneComponent|GetRelativeRotation (Variables|Default|GetWheel)) (Math|Rotator|MakeRotator 0.0 (+ (Variables|Default|GetCurrentUnits) 2.7e+02) 0.0) 0.1 true) false false)))

(fn GetAngleCurrent&MainMesh
  (Utilities|FlowControl|Sequence
    (:then_0
      (bind _returnvalue (CallFunction|GetAngleCurrent&LatestWholeNumVer))
      (LocalVariables|SetDotResult _returnvalue))
    (:then_1
      (bind (_crossvectory _acosd) (CallFunction|GetAngleCurrent&MainMeshWholeNumVer))
      (return _crossvectory _acosd true))))

(fn GetAngleCurrent&LatestWholeNumVer
  (return (Class|KismetMathLibrary|CrossProduct2D (Math|Vector2D|Normalize2D (- (Variables|Default|GetCurrentMousePivot) (Variables|Default|GetViewportCenter))) (Math|Vector2D|Normalize2D (- (+ (Variables|Default|GetViewportCenter) "(X=0.000000,Y=-400.000000)") (Variables|Default|GetViewportCenter))))))

(fn GetAngleCurrent&MainMeshWholeNumVer
  (bind _currentmousepivot (Variables|Default|GetCurrentMousePivot))
  (bind _viewportcenter (Variables|Default|GetViewportCenter))
  (bind _viewportcenter_2 (Variables|Default|GetViewportCenter))
  (bind _viewportcenter_3 (Variables|Default|GetViewportCenter))
  (bind _returnvalue (+ _viewportcenter_2 "(X=0.000000,Y=-400.000000)"))
  (bind _returnvalue_2 (- _currentmousepivot _viewportcenter))
  (bind _returnvalue_3 (Math|Vector2D|Normalize2D _returnvalue_2))
  (bind _returnvalue_4 (- _returnvalue _viewportcenter_3))
  (bind _returnvalue_5 (Math|Vector2D|Normalize2D _returnvalue_4))
  (return (Class|KismetMathLibrary|CrossProduct2D _returnvalue_3 _returnvalue_5) (Class|KismetMathLibrary|DegAcos (Math|Vector2D|DotProduct(2D) _returnvalue_3 _returnvalue_5))))

(fn DragCanceling
  (Variables|Default|SetbReHandle true)
  (if (and (Variables|Default|GetbWholeNumber) (Variables|Default|GetbIsDragging))
    (CallFunction|WholeRotationFixed (Variables|Default|GetbMatchDir)))
  (Variables|Default|SetbIsDragging false)
  (Variables|Default|SetbDragValueIsValid false))

(fn AssignAngletoUnitsInitial
  (params (InputAngle :type Float%20%28double-precision%29))
  (Variables|Default|SetLatestACOSdResult InputAngle)
  (if (and (Variables|Default|GetbContinueRotate) (Variables|Default|GetbMatchDir))
    (Variables|Default|SetCurrentUnits (* (* (Variables|Default|GetAngleUnits) (Variables|Default|GetInsertedGLASSUnits)) -1.0))))

(fn CheckPositiveInput
  (params (CurrentMatchIndex :type Integer))
  (LocalVariables|SetCurrent CurrentMatchIndex)
  (Variables|Default|SetbMatchDir false)
  (Utilities|FlowControl|Sequence
    (:then_0
      (LocalVariables|SetIndexGap (- (LocalVariables|GetCurrent) (Variables|Default|GetLatestMatchIndex)))
      (LocalVariables|SetACOsdGap (- (Variables|Default|GetCurrentACOSdResult) (Variables|Default|GetLatestACOSdResult))))
    (:then_1
      (if (> (LocalVariables|GetIndexGap) 0)
        (LocalVariables|SetbMatch&Update true)
        (elif (== (LocalVariables|GetIndexGap) 0)
          (if (== (LocalVariables|GetCurrent) 0)
            (if (<= (Class|KismetMathLibrary|CrossProduct2D (Math|Vector2D|Normalize2D (- (Variables|Default|GetCurrentMousePivot) (Variables|Default|GetViewportCenter))) (Math|Vector2D|Normalize2D (- (Variables|Default|GetLatestMousePivot) (Variables|Default|GetViewportCenter)))) 0.0)
              (if (< (Variables|Default|GetCurrentACOSdResult) (Variables|Default|GetRangeMin))
                (Variables|Default|SetCurrentACOSdResult (+ (Variables|Default|GetCurrentACOSdResult) 3.6e+02)))
              (if (or (> (- (Variables|Default|GetCurrentACOSdResult) (Variables|Default|GetLatestACOSdResult)) 0.0) (and (== (- (Variables|Default|GetCurrentACOSdResult) (Variables|Default|GetLatestACOSdResult)) 0.0) (Variables|Default|GetbDragValueIsValid)))
                (Variables|Default|SetbDragValueIsValid true)
                (LocalVariables|SetbMatch&Update true)
                (else
                  (LocalVariables|SetbMatch&Update false)
                  (Variables|Default|SetLatestACOSdResult (Variables|Default|GetCurrentACOSdResult))))
              (else
                (LocalVariables|SetbMatch&Update false)))
            (elif (or (> (LocalVariables|GetACOsdGap) 0.0) (and (== (LocalVariables|GetACOsdGap) 0.0) (Variables|Default|GetbDragValueIsValid)))
              (Variables|Default|SetbDragValueIsValid true)
              (LocalVariables|SetbMatch&Update true)
              (else
                (LocalVariables|SetbMatch&Update false)
                (if (< (LocalVariables|GetACOsdGap) 0.0)
                  (Variables|Default|SetLatestACOSdResult (Variables|Default|GetCurrentACOSdResult))))))
          (elif (== (* (LocalVariables|GetIndexGap) -1) (- (Variables|Default|GetDividedCount) 1))
            (LocalVariables|SetbMatch&Update true)
            (else
              (LocalVariables|SetbMatch&Update false))))))
    (:then_2
      (if (LocalVariables|GetbMatch&Update)
        (Variables|Default|SetLatestMatchIndex (LocalVariables|GetCurrent))
        (Variables|Default|SetLatestACOSdResult (Variables|Default|GetCurrentACOSdResult))
        (return true)
        (else
          (return false))))))

(fn BacktoDefault
  (Variables|Default|SetInsertedGLASSUnits -1)
  (CallFunction|AssignAngletoUnitsInitial 0.0)
  (CallFunction|WholeRotationFixedViaUnits true)
  (Variables|Default|SetbDuringReset true)
  (Variables|Default|SetbHasInsertedGLASS false)
  (Default|UpdateGLASSCodefromEachFunc (Variables|Default|GetREF_Collection%20Machine%20Demo%20Beta)))

(fn WholeRotationFixedViaUnits
  (params (bMatchDir :type Boolean))
  (if bMatchDir
    (bind _output_get (Variables|Default|SetResetRot (Math|Rotator|Lerp(Rotator) (Variables|/Script/Engine.SceneComponent|GetRelativeRotation (Variables|Default|GetWheel)) (Math|Rotator|MakeRotator 0.0 (+ (Variables|Default|GetCurrentUnits) 2.7e+02) 0.0) 0.05 true)))
    (Transformation|SetRelativeRotation (Variables|Default|GetWheel) _output_get false false)))

(fn ReceiveGLASScode
  (params (Code :type Integer))
  (Variables|Default|SetInsertedGLASSUnits Code)
  (CallFunction|AssignAngletoUnitsInitial 0.0)
  (CallFunction|WholeRotationFixedViaUnits true)
  (Variables|Default|SetbHasInsertedGLASS true)
  (Default|UpdateGLASSCodefromEachFunc (Variables|Default|GetREF_Collection%20Machine%20Demo%20Beta)))