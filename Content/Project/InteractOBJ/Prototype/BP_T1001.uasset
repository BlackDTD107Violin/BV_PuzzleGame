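; BP_T1001 is a prototype interactable object that can zoom the player's view onto itself and be unlocked by a match code.
; Zooming in blends the view target to this actor, ignores move and look input, and clears the player's prompt UI.
; Zooming out blends back to the character and restores input.
; An unlock event waits briefly, then clears the lock flag if the incoming code matches its set code.
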(event EventBeginPlay
  (|CallParentFunction)
  (bind _asbp_first_person_character (Utilities|Casting|CastToBP_FirstPersonCharacter (Game|GetPlayerCharacter 0)))
  (Variables|Default|SetPlayer _asbp_first_person_character))

(event EventZoomOut
  (bind _returnvalue (Game|GetPlayerController 0))
  (Game|Player|SetViewTargetwithBlend (Game|GetPlayerController 0) (Game|GetPlayerCharacter 0) 0.5 "VTBlend_Linear" 0.0 true)
  (Input|ResetIgnoreMoveInput _returnvalue)
  (Input|ResetIgnoreLookInput _returnvalue))

(event EventInteractiveUnlocked
  (params (AttachKEY :type Actor%20Object%20Reference) (MatchOBJCode :type Name :default "None"))
  (Utilities|FlowControl|Delay 0.2)
  (if (Utilities|Enum|Equal(Enum) (Utilities|String|ToString(Name) MatchOBJCode) (Utilities|String|ToString(Name) (Variables|Default|GetSETMatchCode)))
    (Variables|Default|SetbSTANDIsLocked false)))

(event EventZoomin
  (params (ZoomComponent :type Actor%20Component%20Object%20Reference))
  (bind _returnvalue (Game|GetPlayerController 0))
  (Game|Player|SetViewTargetwithBlend (Game|GetPlayerController 0) self 0.5 "VTBlend_Linear" 0.0 true)
  (Input|SetIgnoreMoveInput _returnvalue true)
  (Input|SetIgnoreLookInput _returnvalue true)
  (Default|ClearGamePromptUIView (Variables|Default|GetPlayer)))

(fn ConstructionScript
  (|CallParentFunction))