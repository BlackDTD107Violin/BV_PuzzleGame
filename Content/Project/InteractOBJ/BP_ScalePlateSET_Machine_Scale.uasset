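; Mouse-dragged slider on the collection machine that sets the inserted GLASS scale as a discrete step.
; While a GLASS is inserted, diagonal mouse drags on the handle step the unit up or down between floor and ceiling.
; Each step lerps the slider height and scale indicator toward target, blocking further steps until settled, and notifies the parent machine to update its GLASS code.
; The unit can also be set from a received code or reset to default.
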(event OnBeginCursorOver(Handler)
  (params (TouchedComponent :type Primitive%20Component%20Object%20Reference))
  (Variables|Default|SetbContinueSlide true)
  (Variables|Default|SetbStillInHandler true))

(event OnEndCursorOver(Handler)
  (params (TouchedComponent :type Primitive%20Component%20Object%20Reference))
  (Utilities|FlowControl|Delay 0.01)
  (Variables|Default|SetbStillInHandler false)
  (if (not (Variables|Default|GetbStillInRail))
    (CallFunction|DragCanceling)))

(event OnClicked(Handler)
  (params (TouchedComponent :type Primitive%20Component%20Object%20Reference) (ButtonPressed :type Key%20Structure :default "None"))
  (Variables|Default|SetbIsDragging true))

(event OnReleased(Handler)
  (params (TouchedComponent :type Primitive%20Component%20Object%20Reference) (ButtonReleased :type Key%20Structure :default "None"))
  (CallFunction|DragCanceling))

(event OnBeginCursorOver(RailTA)
  (params (TouchedComponent :type Primitive%20Component%20Object%20Reference))
  (Variables|Default|SetbStillInRail true))

(event OnEndCursorOver(RailTA)
  (params (TouchedComponent :type Primitive%20Component%20Object%20Reference))
  (Utilities|FlowControl|Delay 0.01)
  (if (not (Variables|Default|GetbStillInHandler))
    (CallFunction|DragCanceling)
    (Variables|Default|SetbStillInRail false)))

(event OnReleased(RailTA)
  (params (TouchedComponent :type Primitive%20Component%20Object%20Reference) (ButtonReleased :type Key%20Structure :default "None"))
  (CallFunction|DragCanceling)
  (Variables|Default|SetbStillInRail false))

(event EventBeginPlay
  (bind _returnvalue (Game|GetPlayerController 0))
  (|CallParentFunction)
  (bind _asbp_first_person_character (Utilities|Casting|CastToBP_FirstPersonCharacter (Game|GetPlayerCharacter 0)))
  (Variables|Default|SetPlayer _asbp_first_person_character)
  (Input|EnableInput _returnvalue)
  (Variables|/Script/Engine.PlayerController|SetbEnableClickEvents _returnvalue true)
  (Variables|/Script/Engine.PlayerController|SetbEnableMouseOverEvents _returnvalue true)
  (bind _asbp_collection_machine_demo_beta (Utilities|Casting|CastToBP_CollectionMachineDemo_beta (Actor|GetParentActor)))
  (Variables|Default|SetREF_Collection%20Machine%20Demo%20Beta _asbp_collection_machine_demo_beta)
  (CallFunction|InitialSlideState)
  (CallFunction|AssignPosUnits)
  (CallFunction|WholePositionFixed))

(event EventTick
  (params (DeltaSeconds :type Float%20%28single-precision%29))
  (if (Variables|Default|GetbHasInsertedGLASS)
    (if (Variables|Default|GetbIsDragging)
      (bind (_bhascrossedrange _bscalingdir) (CallFunction|UpdatePlayerInput))
      (if _bhascrossedrange
        (CallFunction|AssignWidthUnits _bscalingdir)
        (CallFunction|WholePositionFixed))
      (else
        (CallFunction|WholePositionFixed :!label _label)))
    (else
      (goto _label))))

(fn ConstructionScript
  (|CallParentFunction))

(fn AssignPosUnits
  (LocalVariables|SetInitPos (.z (Variables|Default|GetOriginPos)))
  (bind _index (Utilities|FlowControl|ForLoopwithBreak 0 (- (Variables|Default|GetDividedCount) 1) :!label _label)
    (:LoopBody
      (bind _targetunit (CallFunction|DivideRangeLooping _index))
      (bind _bfound (CallFunction|CheckPosRange (LocalVariables|GetInitPos) _index _targetunit))
      (if _bfound
        (goto _label Break)))))

(fn AssignWidthUnits
  (params (bScalingDir :type Boolean))
  (if bScalingDir
    (if (and (Variables|Default|GetbContinueSlide) (not (Variables|Default|GetbDuringFixing)))
      (if (not (Variables|Default|GetbReachCeiling))
        (bind _result (Math|Integer|IncrementInt (Variables|Default|GetInsertedGLASSUnits))
          (:%20%20
            (bind _output_get (Variables|Default|SetInsertedGLASSUnits _result))
            (if (== _output_get (- (Variables|Default|GetDividedCount) 1))
              (Variables|Default|SetbReachCeiling true)
              (Variables|Default|SetbDuringFixing true)
              (Default|UpdateGLASSCodefromEachFunc (Variables|Default|GetREF_Collection%20Machine%20Demo%20Beta))
              (else
                (Variables|Default|SetbReachFloor false)
                (Variables|Default|SetbDuringFixing true)
                (Default|UpdateGLASSCodefromEachFunc (Variables|Default|GetREF_Collection%20Machine%20Demo%20Beta))))))))
    (elif (and (Variables|Default|GetbContinueSlide) (not (Variables|Default|GetbDuringFixing)))
      (if (not (Variables|Default|GetbReachFloor))
        (bind _result_2 (Math|Integer|DecrementInt (Variables|Default|GetInsertedGLASSUnits))
          (:%20%20
            (bind _output_get_2 (Variables|Default|SetInsertedGLASSUnits _result_2))
            (if (== _output_get_2 0)
              (Variables|Default|SetbReachFloor true)
              (Variables|Default|SetbDuringFixing true)
              (Default|UpdateGLASSCodefromEachFunc (Variables|Default|GetREF_Collection%20Machine%20Demo%20Beta))
              (else
                (Variables|Default|SetbReachCeiling false)
                (Variables|Default|SetbDuringFixing true)
                (Default|UpdateGLASSCodefromEachFunc (Variables|Default|GetREF_Collection%20Machine%20Demo%20Beta))))))))))

(fn CheckPosRange
  (params (InputAngle :type Float%20%28double-precision%29) (Index :type Integer) (TargetUnits :type Float%20%28double-precision%29))
  (LocalVariables|SetInput InputAngle)
  (Variables|Default|SetInsertedGLASSUnits Index)
  (Default|UpdateGLASSCodefromEachFunc (Variables|Default|GetREF_Collection%20Machine%20Demo%20Beta))
  (if (and (> (LocalVariables|GetInput) (Variables|Default|GetRangeMin)) (<= (LocalVariables|GetInput) (Variables|Default|GetRangeMax)))
    (Variables|Default|SetbReachFloor (== (Variables|Default|GetInsertedGLASSUnits) 0))
    (Variables|Default|SetbReachCeiling (== (Variables|Default|GetInsertedGLASSUnits) (- (Variables|Default|GetDividedCount) 1)))
    (return true)
    (else
      (return false))))

(fn DivideRangeLooping
  (params (DevidedCount :type Integer))
  (LocalVariables|SetTargetUnits (+ (* DevidedCount (Variables|Default|GetSlideUnits)) (+ (.z (Variables|Default|GetOriginPos)) (Variables|Default|GetSlideCeiling))))
  (Utilities|FlowControl|Sequence
    (:then_0
      (Variables|Default|SetRangeMax (+ (LocalVariables|GetTargetUnits) (/ (Variables|Default|GetSlideUnits) 2.0))))
    (:then_1
      (Variables|Default|SetRangeMin (- (LocalVariables|GetTargetUnits) (/ (Variables|Default|GetSlideUnits) 2.0))))
    (:then_2
      (return (LocalVariables|GetTargetUnits)))))

(fn DragCanceling
  (Variables|Default|SetbIsDragging false)
  (Variables|Default|SetbReHandle true)
  (CallFunction|WholePositionFixed))

(fn InitialSlideState
  (bind _returnvalue (Game|GetPlayerController 0))
  (bind (_sizex _sizey) (HUD|GetViewportSize _returnvalue))
  (Utilities|FlowControl|Sequence
    (:then_0
      (Variables|Default|SetOriginPos (Variables|/Script/Engine.SceneComponent|GetRelativeLocation (Variables|Default|GetSlider)))
      (Variables|Default|SetScreenWidth _sizex)
      (Variables|Default|SetScreenHeight _sizey))
    (:then_1
      (Variables|Default|SetSlideUnits (/ (- (Variables|Default|GetSlideFloor) (Variables|Default|GetSlideCeiling)) (Variables|Default|GetDividedCount)))
      (Variables|Default|SetScreenWidthUnits (Math|Conversions|ToFloat(Integer) (/ (Variables|Default|GetScreenWidth) 100)))
      (Variables|Default|SetScreenHeightUnits (Math|Conversions|ToFloat(Integer) (/ (Variables|Default|GetScreenHeight) 100))))))

(fn UpdatePlayerInput
  (bind _returnvalue (Game|GetPlayerController 0))
  (bind _bisinview (CallFunction|CheckPlayerInputinView))
  (if _bisinview
    (Variables|Default|SetCurrentMousePivot (.ScreenLocation (Class|PlayerController|ProjectWorldLocationtoScreen _returnvalue (.WorldLocation (Game|Player|ConvertMouseLocationToWorldSpace _returnvalue)) false)))
    (if (Variables|Default|GetbReHandle)
      (Variables|Default|SetbReHandle false)
      (Variables|Default|SetLatestMousePivot (Variables|Default|GetCurrentMousePivot))
      (return false false)
      (elif (and (> (.X (Math|Vector2D|BreakVector2D (- (Variables|Default|GetCurrentMousePivot) (Variables|Default|GetLatestMousePivot)))) 0.0) (> (.Y (Math|Vector2D|BreakVector2D (- (Variables|Default|GetCurrentMousePivot) (Variables|Default|GetLatestMousePivot)))) 0.0))
        (return true true)
        (elif (and (< (.X (Math|Vector2D|BreakVector2D (- (Variables|Default|GetCurrentMousePivot) (Variables|Default|GetLatestMousePivot)))) 0.0) (< (.Y (Math|Vector2D|BreakVector2D (- (Variables|Default|GetCurrentMousePivot) (Variables|Default|GetLatestMousePivot)))) 0.0))
          (return true false)
          (else
            (return false false)))))
    (else
      (return false false))))

(fn WholePositionFixed
  (bind _returnvalue (Game|GetPlayerController 0))
  (bind _returnvaluez (CallFunction|GetTargetPos))
  (LocalVariables|SetTargetPosZ _returnvaluez)
  (if (Variables|Default|GetbDuringFixing)
    (CallFunction|BlendtoTargetPos (LocalVariables|GetTargetPosZ))
    (CallFunction|BlendtoTargetScale)
    (bind _output_get (CallFunction|CheckIsDuringFixing (LocalVariables|GetTargetPosZ)))
    (bind _output_get_2 (Variables|Default|SetbDuringFixing _output_get))
    (if (not _output_get_2)
      (Variables|Default|SetLatestMousePivot (.ScreenLocation (Class|PlayerController|ProjectWorldLocationtoScreen _returnvalue (.WorldLocation (Game|Player|ConvertMouseLocationToWorldSpace _returnvalue)) false))))))

(fn GetTargetPos
  (return (- (+ (.z (Variables|Default|GetOriginPos)) (Variables|Default|GetSlideFloor)) (* (Variables|Default|GetInsertedGLASSUnits) (Variables|Default|GetSlideUnits)))))

(fn BlendtoTargetPos
  (params (TargetPosZ :type Float%20%28double-precision%29))
  (bind _slider (Variables|Default|GetSlider))
  (bind _relativelocation (Variables|/Script/Engine.SceneComponent|GetRelativeLocation _slider))
  (Transformation|SetRelativeLocation (Variables|Default|GetSlider) (Math|Vector|Lerp(Vector) (Variables|/Script/Engine.SceneComponent|GetRelativeLocation (Variables|Default|GetSlider)) (Math|Vector|MakeVector (.x _relativelocation) (.y _relativelocation) TargetPosZ) 0.25) false false))

(fn BlendtoTargetScale
  (bind _insertedglassunits (Variables|Default|GetInsertedGLASSUnits))
  (bind _returnvalue (Math|Conversions|ToFloat(Integer) _insertedglassunits))
  (bind _returnvalue_2 (* _returnvalue 0.2))
  (bind _returnvalue_3 (+ _returnvalue_2 0.2))
  (Transformation|SetRelativeScale3D (Variables|Default|GetScalingIndex) (Math|Vector|Lerp(Vector) (Variables|/Script/Engine.SceneComponent|GetRelativeScale3D (Variables|Default|GetScalingIndex)) (Math|Vector|MakeVector _returnvalue_3 _returnvalue_3 (.z (Variables|/Script/Engine.SceneComponent|GetRelativeScale3D (Variables|Default|GetScalingIndex)))) 0.25)))

(fn CheckIsDuringFixing
  (params (TargetPosZ :type Float%20%28double-precision%29))
  (bind _returnvalue (Math|Vector|MakeVector 0.0 0.0 TargetPosZ))
  (bind _slider (Variables|Default|GetSlider))
  (bind _relativelocation (Variables|/Script/Engine.SceneComponent|GetRelativeLocation _slider))
  (bind _returnvalue_2 (- (.z _relativelocation) (.z _returnvalue)))
  (return (not (and (<= _returnvalue_2 0.001) (>= _returnvalue_2 -0.001)))))

(fn CheckPlayerInputinView
  (bind _returnvalue (Game|GetPlayerController 0))
  (bind _returnvalue_2 (Game|GetPlayerController 0))
  (bind _worldlocation (Game|Player|ConvertMouseLocationToWorldSpace _returnvalue))
  (bind _worldlocation_2 (Game|Player|ConvertMouseLocationToWorldSpace _returnvalue_2))
  (bind _screenlocation (Class|PlayerController|ProjectWorldLocationtoScreen _returnvalue _worldlocation false))
  (bind _screenlocation_2 (Class|PlayerController|ProjectWorldLocationtoScreen _returnvalue_2 _worldlocation_2 false))
  (return (and (and (>= (.x _screenlocation_2) 0.0) (<= (.x _screenlocation_2) (.SizeX (HUD|GetViewportSize (Game|GetPlayerController 0))))) (and (>= (.y _screenlocation) 0.0) (<= (.y _screenlocation) (.SizeY (HUD|GetViewportSize (Game|GetPlayerController 0))))))))

(fn BacktoDefault
  (Variables|Default|SetInsertedGLASSUnits 3)
  (CallFunction|WholePositionFixedViaUnits)
  (Variables|Default|SetbHasInsertedGLASS false)
  (Default|UpdateGLASSCodefromEachFunc (Variables|Default|GetREF_Collection%20Machine%20Demo%20Beta)))

(fn WholePositionFixedViaUnits
  (bind _returnvalue (Game|GetPlayerController 0))
  (bind _returnvaluez (CallFunction|GetTargetPos))
  (LocalVariables|SetTargetPosZ _returnvaluez)
  (CallFunction|BlendtoTargetPos (LocalVariables|GetTargetPosZ))
  (CallFunction|BlendtoTargetScale)
  (bind _output_get (CallFunction|CheckIsDuringFixing (LocalVariables|GetTargetPosZ)))
  (bind _output_get_2 (Variables|Default|SetbDuringFixing _output_get))
  (if (not _output_get_2)
    (Variables|Default|SetLatestMousePivot (.ScreenLocation (Class|PlayerController|ProjectWorldLocationtoScreen _returnvalue (.WorldLocation (Game|Player|ConvertMouseLocationToWorldSpace _returnvalue)) false)))))

(fn ReceiveGLASScode
  (params (Code :type Integer))
  (Variables|Default|SetInsertedGLASSUnits Code)
  (CallFunction|WholePositionFixedViaUnits)
  (Variables|Default|SetbHasInsertedGLASS true)
  (Default|UpdateGLASSCodefromEachFunc (Variables|Default|GetREF_Collection%20Machine%20Demo%20Beta)))