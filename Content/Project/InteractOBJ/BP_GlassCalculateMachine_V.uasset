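; Interactable glass calculate machine with a sliding drawer that holds a glass notch, linked to a gear slider.
; Tick either auto-slides the drawer open or closed, or lets mouse drags push it closed, interpolating to the nearest end on release near either limit.
; End states play sounds and variously toggle collision, refresh the notch's totem and panel, or reset the slider.
; Child-actor references are wired at BeginPlay, and inserted glass is forwarded to the slider bar.
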(event OnClicked(Drawer)
  (params (TouchedComponent :type Primitive%20Component%20Object%20Reference) (ButtonPressed :type Key%20Structure :default "None"))
  (Variables|Default|SetbIsDraggingDrawer true)
  (Variables|/Game/ProjectDefault/FirstPerson/Blueprints/BP_FirstPersonCharacter.BP_FirstPersonCharacter_C|SetCurrentInteract (Variables|Default|GetPlayer) self))

(event Custom|ResetSlider
  (Utilities|FlowControl|Delay 0.5)
  (bind _asbp_gear_with_slider_test (Utilities|Casting|CastToBP_GearWithSliderTest (Variables|/Script/Engine.ChildActorComponent|GetChildActor (Variables|Default|GetGear))))
  (bind _asbp_gear_slider_bar (Utilities|Casting|CastToBP_GearSliderBar (Variables|/Script/Engine.ChildActorComponent|GetChildActor (Variables|/Game/Project/InteractOBJ/BP_GearWithSliderTest.BP_GearWithSliderTest_C|GetSlider _asbp_gear_with_slider_test))))
  (Variables|/Game/Project/InteractOBJ/BP_GearSliderBar.BP_GearSliderBar_C|SetbSlideBarIsFinish _asbp_gear_slider_bar false))

(event EventBeginPlay
  (bind _returnvalue (Game|GetPlayerController 0))
  (|CallParentFunction)
  (bind _asbp_first_person_character (Utilities|Casting|CastToBP_FirstPersonCharacter (Game|GetPlayerCharacter 0)))
  (Variables|Default|SetPlayer _asbp_first_person_character)
  (Input|EnableInput _returnvalue)
  (Variables|/Script/Engine.PlayerController|SetbEnableClickEvents _returnvalue true)
  (Variables|/Script/Engine.PlayerController|SetbEnableMouseOverEvents _returnvalue true)
  (CallFunction|PresetChildActor))

(event EventTick
  (params (DeltaSeconds :type Float%20%28single-precision%29))
  (if (Variables|Default|GetbDrawerIsAuto)
    (CallFunction|DrawerAutoMode (Variables|Default|GetbIsAutoOpen))
    (else
      (CallFunction|DrawerPlayerMode))))

(event Input|MouseEvents|LeftMouseButton
  (params (Key :type Key%20Structure :default "None"))
  (:Released
    (if (== (Variables|/Game/ProjectDefault/FirstPerson/Blueprints/BP_FirstPersonCharacter.BP_FirstPersonCharacter_C|GetCurrentInteract (Variables|Default|GetPlayer)) self)
      (if (Variables|Default|GetbIsDraggingDrawer)
        (Variables|Default|SetbIsDraggingDrawer false)))))

(fn ConstructionScript
  (|CallParentFunction))

(fn AutoOpenDrawer
  (bind _drawer (Variables|Default|GetDrawer))
  (bind _relativelocation (Variables|/Script/Engine.SceneComponent|GetRelativeLocation _drawer))
  (Transformation|AddLocalOffset (Variables|Default|GetDrawer) (Math|Vector|MakeVector 0.0 (Variables|Default|GetDefaultSpeed) 0.0) false false)
  (if (>= (.y (Variables|/Script/Engine.SceneComponent|GetRelativeLocation (Variables|Default|GetDrawer))) 25.0)
    (Transformation|SetRelativeLocation _drawer (Math|Vector|MakeVector (.x _relativelocation) 25.0 (.z _relativelocation)) false false)
    (Variables|Default|SetbHasUpdateMouseDrawerPivot false)
    (if (not (Variables|Default|GetDrawer_WholeState))
      (Variables|Default|SetDrawer_WholeState true)
      (Audio|SpawnSoundAttached "/Game/Project/Audio/MetaSoundSource/MSS_S0003_LockFinish.MSS_S0003_LockFinish" (Variables|Default|GetDrawer) "None" "0, 0, 0" "0, 0, 0" "KeepRelativeOffset" false 1.0 1.0 0.0 0 0)
      (Variables|Default|SetbSoundPlaying false)
      (Variables|Default|SetbDrawerIsAuto false)
      (Collision|SetCollisionProfileName (Variables|Default|GetDrawer) "BlockAllDynamic" true :!class /Script/Engine.PrimitiveComponent)
      (Variables|Default|SetbAutoOpenDrawer false)
      (Default|CollisionbyAutoState (Variables|Default|GetREF_GlassNotch_V) true))
    (else
      (CallFunction|UpdateTriggerMousePivot)
      (Variables|Default|SetDrawer_WholeState false)
      (if (not (Variables|Default|GetbSoundPlaying))
        (Variables|Default|SetbSoundPlaying true)
        (Audio|SpawnSoundAttached "/Game/Project/Audio/MetaSoundSource/MSS_S0003_LockSlide.MSS_S0003_LockSlide" (Variables|Default|GetDrawer) "None" "0, 0, 0" "0, 0, 0" "KeepRelativeOffset" false 1.0 1.0 0.0 0 0)))))

(fn AutoCloseDrawer
  (bind _drawer (Variables|Default|GetDrawer))
  (bind _relativelocation (Variables|/Script/Engine.SceneComponent|GetRelativeLocation _drawer))
  (Transformation|AddLocalOffset (Variables|Default|GetDrawer) (Math|Vector|MakeVector 0.0 (* (Variables|Default|GetDefaultSpeed) -1.0) 0.0) false false)
  (if (<= (.y (Variables|/Script/Engine.SceneComponent|GetRelativeLocation (Variables|Default|GetDrawer))) 0.0)
    (Transformation|SetRelativeLocation _drawer (Math|Vector|MakeVector (.x _relativelocation) 0.0 (.z _relativelocation)) false false)
    (Variables|Default|SetbHasUpdateMouseDrawerPivot false)
    (if (not (Variables|Default|GetDrawer_WholeState))
      (Variables|Default|SetDrawer_WholeState true)
      (Audio|SpawnSoundAttached "/Game/Project/Audio/MetaSoundSource/MSS_S0003_LockFinish.MSS_S0003_LockFinish" (Variables|Default|GetDrawer) "None" "0, 0, 0" "0, 0, 0" "KeepRelativeOffset" false 1.0 1.0 0.0 0 0)
      (Variables|Default|SetbSoundPlaying false)
      (Variables|Default|SetbDrawerIsAuto false)
      (Collision|SetCollisionProfileName (Variables|Default|GetDrawer) "NoCollision" true :!class /Script/Engine.PrimitiveComponent)
      (Variables|Default|SetbAutoOpenDrawer false)
      (Default|CollisionbyAutoState (Variables|Default|GetREF_GlassNotch_V) false)
      (Default|UpdateTotemandPanel (Variables|/Game/Project/InteractOBJ/BP_GLASSnotch_Mix.BP_GLASSnotch_Mix_C|GetREF_OBJ%20TA (Variables|Default|GetREF_GlassNotch_V))))
    (else
      (CallFunction|UpdateTriggerMousePivot)
      (Variables|Default|SetDrawer_WholeState false)
      (if (not (Variables|Default|GetbSoundPlaying))
        (Variables|Default|SetbSoundPlaying true)
        (Audio|SpawnSoundAttached "/Game/Project/Audio/MetaSoundSource/MSS_S0003_LockSlide.MSS_S0003_LockSlide" (Variables|Default|GetDrawer) "None" "0, 0, 0" "0, 0, 0" "KeepRelativeOffset" false 1.0 1.0 0.0 0 0)))))

(fn DrawerAutoMode
  (params (bIsOpen :type Boolean))
  (if bIsOpen
    (CallFunction|AutoOpenDrawer)
    (else
      (CallFunction|AutoCloseDrawer))))

(fn DrawerPlayerMode
  (bind _drawer (Variables|Default|GetDrawer))
  (bind _relativelocation (Variables|/Script/Engine.SceneComponent|GetRelativeLocation _drawer))
  (if (Variables|Default|GetbIsDraggingDrawer)
    (if (Variables|Default|GetbHasUpdateMouseDrawerPivot)
      (CallFunction|DragDrawerViaInput)
      (else
        (Variables|Default|SetbHasUpdateMouseDrawerPivot true)
        (CallFunction|UpdateTriggerMousePivot)))
    (elif (>= (.y _relativelocation) 2e+01)
      (CallFunction|FinishRemainingOffsetDrawer true)
      (elif (<= (.y _relativelocation) 5.0)
        (CallFunction|FinishRemainingOffsetDrawer false)))))

(fn PresetChildActor
  (Utilities|FlowControl|Sequence
    (:then_0
      (bind _asbp_gear_with_slider_test (Utilities|Casting|CastToBP_GearWithSliderTest (Variables|/Script/Engine.ChildActorComponent|GetChildActor (Variables|Default|GetGear))))
      (bind _asbp_gear_slider_bar (Utilities|Casting|CastToBP_GearSliderBar (Variables|/Script/Engine.ChildActorComponent|GetChildActor (Variables|/Game/Project/InteractOBJ/BP_GearWithSliderTest.BP_GearWithSliderTest_C|GetSlider _asbp_gear_with_slider_test))))
      (Variables|/Game/Project/InteractOBJ/BP_GearSliderBar.BP_GearSliderBar_C|SetREF_CalculateMachine _asbp_gear_slider_bar self))
    (:then_1
      (bind _asbp_glassnotch_v (Utilities|Casting|CastToBP_GLASSnotch_V (Variables|/Script/Engine.ChildActorComponent|GetChildActor (Variables|Default|GetGlassNotch_V))))
      (Variables|Default|SetREF_GlassNotch_V _asbp_glassnotch_v))))

(fn UpdateTriggerMousePivot
  (bind _returnvalue (Game|GetPlayerController 0))
  (Variables|Default|SetTriggerMousePivot (.ScreenLocation (Class|PlayerController|ProjectWorldLocationtoScreen _returnvalue (.WorldLocation (Game|Player|ConvertMouseLocationToWorldSpace _returnvalue)) false))))

(fn DragDrawerViaInput
  (bind _returnvalue (Game|GetPlayerController 0))
  (bind _drawer (Variables|Default|GetDrawer))
  (bind _triggermousepivot (Variables|Default|GetTriggerMousePivot))
  (bind _worldlocation (Game|Player|ConvertMouseLocationToWorldSpace _returnvalue))
  (bind _relativelocation (Variables|/Script/Engine.SceneComponent|GetRelativeLocation _drawer))
  (bind _screenlocation (Class|PlayerController|ProjectWorldLocationtoScreen _returnvalue _worldlocation false))
  (if (!= (.y _screenlocation) (.y _triggermousepivot))
    (if (not (> (.y _screenlocation) (.y _triggermousepivot)))
      (Transformation|AddLocalOffset (Variables|Default|GetDrawer) (Math|Vector|MakeVector 0.0 (* (Variables|Default|GetDefaultSpeed) -1.0) 0.0) false false)
      (if (<= (.y (Variables|/Script/Engine.SceneComponent|GetRelativeLocation (Variables|Default|GetDrawer))) 0.0)
        (Transformation|SetRelativeLocation _drawer (Math|Vector|MakeVector (.x _relativelocation) 0.0 (.z _relativelocation)) false false)
        (Variables|Default|SetbHasUpdateMouseDrawerPivot false)
        (if (not (Variables|Default|GetDrawer_WholeState))
          (Variables|Default|SetDrawer_WholeState true)
          (Audio|SpawnSoundAttached "/Game/Project/Audio/MetaSoundSource/MSS_S0003_LockFinish.MSS_S0003_LockFinish" (Variables|Default|GetDrawer) "None" "0, 0, 0" "0, 0, 0" "KeepRelativeOffset" false 1.0 1.0 0.0 0 0)
          (Variables|Default|SetbSoundPlaying false)
          (Variables|Default|SetbDrawerIsAuto false)
          (Collision|SetCollisionProfileName (Variables|Default|GetDrawer) "NoCollision" true :!class /Script/Engine.PrimitiveComponent)
          (Variables|Default|SetbAutoOpenDrawer false)
          (Default|CollisionbyAutoState (Variables|Default|GetREF_GlassNotch_V) false)
          (CallFunction|ResetSlider))
        (else
          (CallFunction|UpdateTriggerMousePivot)
          (Variables|Default|SetDrawer_WholeState false)
          (if (not (Variables|Default|GetbSoundPlaying))
            (Variables|Default|SetbSoundPlaying true)
            (Audio|SpawnSoundAttached "/Game/Project/Audio/MetaSoundSource/MSS_S0003_LockSlide.MSS_S0003_LockSlide" (Variables|Default|GetDrawer) "None" "0, 0, 0" "0, 0, 0" "KeepRelativeOffset" false 1.0 1.0 0.0 0 0)))))))

(fn FinishRemainingOffsetDrawer
  (params (bGoingOpen :type Boolean))
  (bind _drawer (Variables|Default|GetDrawer))
  (bind _drawer_2 (Variables|Default|GetDrawer))
  (bind _relativelocation (Variables|/Script/Engine.SceneComponent|GetRelativeLocation _drawer_2))
  (bind _relativelocation_2 (Variables|/Script/Engine.SceneComponent|GetRelativeLocation _drawer))
  (bind _output_get (LocalVariables|SetL_GoingOpen bGoingOpen))
  (if _output_get
    (LocalVariables|SetL_TargetPos 25.0)
    (LocalVariables|SetL_TouchPos 24.0)
    (else
      (LocalVariables|SetL_TargetPos 0.0)
      (LocalVariables|SetL_TouchPos 1.0)))
  (Utilities|FlowControl|Sequence
    (:then_0
      (Transformation|SetRelativeLocation (Variables|Default|GetDrawer) (Math|Interpolation|VInterpTo (Variables|/Script/Engine.SceneComponent|GetRelativeLocation (Variables|Default|GetDrawer)) (Math|Vector|MakeVector (.x _relativelocation_2) (LocalVariables|GetL_TargetPos) (.z _relativelocation_2)) (Utilities|Time|GetWorldDeltaSeconds) 4.0) false false))
    (:then_1
      (if (and (LocalVariables|GetL_GoingOpen) (>= (.y (Variables|/Script/Engine.SceneComponent|GetRelativeLocation (Variables|Default|GetDrawer))) (LocalVariables|GetL_TouchPos)))
        (Transformation|SetRelativeLocation _drawer_2 (Math|Vector|MakeVector (.x _relativelocation) (LocalVariables|GetL_TargetPos) (.z _relativelocation)) false false :!label _label)
        (Variables|Default|SetbHasUpdateMouseDrawerPivot false)
        (if (not (Variables|Default|GetDrawer_WholeState))
          (Variables|Default|SetDrawer_WholeState true)
          (Audio|SpawnSoundAttached "/Game/Project/Audio/MetaSoundSource/MSS_S0003_LockFinish.MSS_S0003_LockFinish" (Variables|Default|GetDrawer) "None" "0, 0, 0" "0, 0, 0" "KeepRelativeOffset" false 1.0 1.0 0.0 0 0)
          (Variables|Default|SetbSoundPlaying false)
          (if (not (LocalVariables|GetL_GoingOpen))
            (Default|UpdateTotemandPanel (Variables|/Game/Project/InteractOBJ/BP_GLASSnotch_Mix.BP_GLASSnotch_Mix_C|GetREF_OBJ%20TA (Variables|Default|GetREF_GlassNotch_V)))
            (CallFunction|ResetSlider)))
        (elif (and (not (LocalVariables|GetL_GoingOpen)) (<= (.y (Variables|/Script/Engine.SceneComponent|GetRelativeLocation (Variables|Default|GetDrawer))) (LocalVariables|GetL_TouchPos)))
          (goto _label))))))

(fn GlassHasInserted
  (params (GlassInserted :type BP%20GLASS%20Item%20Object%20Reference))
  (bind _asbp_gear_with_slider_test (Utilities|Casting|CastToBP_GearWithSliderTest (Variables|/Script/Engine.ChildActorComponent|GetChildActor (Variables|Default|GetGear))))
  (bind _asbp_gear_slider_bar (Utilities|Casting|CastToBP_GearSliderBar (Variables|/Script/Engine.ChildActorComponent|GetChildActor (Variables|/Game/Project/InteractOBJ/BP_GearWithSliderTest.BP_GearWithSliderTest_C|GetSlider _asbp_gear_with_slider_test))))
  (Utilities|Array|Add (Variables|/Game/Project/Core/InteractOBJ/BP_CoreOBJ_SET.BP_CoreOBJ_SET_C|GetSETLists _asbp_gear_slider_bar) GlassInserted))