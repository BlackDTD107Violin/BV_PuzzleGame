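; Glass slot actor for the mix machine, spawned as a child actor of a glass placement set.
; On BeginPlay it caches its parent placement actor to reach the mix machine.
; RefreshInsertedGLASS sends an inserted glass to the machine with a fixed notch side, triggers the placement's Interact, links the glass back to itself, then makes it visible and collidable.
; BASE and UNITE types share identical handling; calculate-machine logic remains unconnected.
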(event EventBeginPlay
  (bind _asbp_set_glassplace_mix_machine (Utilities|Casting|CastToBP_SET_GLASSplace_MixMachine (Actor|GetParentActor)))
  (Variables|Default|SetREF%20SET%20GLASSplace%20Mix%20Machine _asbp_set_glassplace_mix_machine))

(fn ConstructionScript)

(fn RefreshInsertedGLASS
  (params (InsertedGlass :type ST%20Glass%20Base%20Collection%20Structure) (InsertedType :type E_GLASSType%20Enum :default "NewEnumerator6"))
  (Variables|Default|SetInsertedGlass InsertedGlass)
  (switch Utilities|FlowControl|Switch|SwitchonE_GLASSType InsertedType
    (:NewEnumerator6
      (Default|ReceiveGLASSCode (Variables|/Game/Project/InteractOBJ/BP_SET_GLASSplace_MixMachine.BP_SET_GLASSplace_MixMachine_C|GetREF_GlassMixMachine (Variables|Default|GetREF%20SET%20GLASSplace%20Mix%20Machine)) (Variables|Default|GetInsertedGlass) "NewEnumerator0")
      (Default|Interact (Variables|Default|GetREF%20SET%20GLASSplace%20Mix%20Machine) (.TargetGlassActor (Utilities|Struct|BreakST_GlassBaseCollection (Variables|Default|GetInsertedGlass))))
      (Variables|/Game/Project/Core/InteractOBJ/BP_CoreOBJ_GLASS.BP_CoreOBJ_GLASS_C|SetCurrentInsertedGLASSMixTA (.TargetGlassActor (Utilities|Struct|BreakST_GlassBaseCollection (Variables|Default|GetInsertedGlass))) self)
      (Rendering|SetActorHiddenInGame (.TargetGlassActor (Utilities|Struct|BreakST_GlassBaseCollection (Variables|Default|GetInsertedGlass))) false)
      (Collision|SetActorEnableCollision (.TargetGlassActor (Utilities|Struct|BreakST_GlassBaseCollection (Variables|Default|GetInsertedGlass))) true))
    (:NewEnumerator1
      (Default|ReceiveGLASSCode (Variables|/Game/Project/InteractOBJ/BP_SET_GLASSplace_MixMachine.BP_SET_GLASSplace_MixMachine_C|GetREF_GlassMixMachine (Variables|Default|GetREF%20SET%20GLASSplace%20Mix%20Machine)) (Variables|Default|GetInsertedGlass) "NewEnumerator0")
      (Default|Interact (Variables|Default|GetREF%20SET%20GLASSplace%20Mix%20Machine) (.TargetGlassActor (Utilities|Struct|BreakST_GlassBaseCollection (Variables|Default|GetInsertedGlass))))
      (Variables|/Game/Project/Core/InteractOBJ/BP_CoreOBJ_GLASS.BP_CoreOBJ_GLASS_C|SetCurrentInsertedGLASSMixTA (.TargetGlassActor (Utilities|Struct|BreakST_GlassBaseCollection (Variables|Default|GetInsertedGlass))) self)
      (Rendering|SetActorHiddenInGame (.TargetGlassActor (Utilities|Struct|BreakST_GlassBaseCollection (Variables|Default|GetInsertedGlass))) false)
      (Collision|SetActorEnableCollision (.TargetGlassActor (Utilities|Struct|BreakST_GlassBaseCollection (Variables|Default|GetInsertedGlass))) true))))