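; Tilt maze object whose BasePlate tilts to follow the mouse cursor's offset from the screen center.
; Each Tick, TiltDetect gets the cursor position by deprojecting and reprojecting it, then TiltAxisX and TiltAxisY scale it to LimitedRange as roll and pitch.
; Each axis holds its last tilt inside the screen-edge padding.
; The plate eases toward the target with a fixed-alpha, frame-rate-dependent lerp, around a 90-degree roll offset.
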(event EventBeginPlay
  (bind _returnvalue (Viewport|GetViewportSize))
  (|CallParentFunction)
  (Variables|Default|SetScreenCenterPivot (Math|Vector2D|MakeVector2D (/ (.x _returnvalue) 2.0) (/ (.y _returnvalue) 2.0))))

(event EventTick
  (params (DeltaSeconds :type Float%20%28single-precision%29))
  (CallFunction|TiltDetect))

(fn ConstructionScript
  (|CallParentFunction))

(fn TiltDetect
  (bind _returnvalue (Game|GetPlayerController 0))
  (bind _worldlocation (Game|Player|ConvertMouseLocationToWorldSpace _returnvalue))
  (bind _screenlocation (Class|PlayerController|ProjectWorldLocationtoScreen _returnvalue _worldlocation false))
  (Utilities|FlowControl|Sequence
    (:then_0
      (Variables|Default|SetCurrentTiltX (.x _screenlocation))
      (Variables|Default|SetCurrentTiltY (.y _screenlocation)))
    (:then_1
      (bind _tiltx (CallFunction|TiltAxisX))
      (bind _tilty (CallFunction|TiltAxisY))
      (Transformation|SetRelativeRotation (Variables|Default|GetBasePlate) (Math|Rotator|Lerp(Rotator) (Variables|/Script/Engine.SceneComponent|GetRelativeRotation (Variables|Default|GetBasePlate)) (Math|Rotator|MakeRotator (+ _tiltx 9e+01) _tilty 0.0) 0.1 true) false false))))

(fn TiltAxisX
  (if (or (>= (Variables|Default|GetCurrentTiltX) (- (.x (Viewport|GetViewportSize)) (Variables|Default|GetPaddingLimited))) (<= (Variables|Default|GetCurrentTiltX) (Variables|Default|GetPaddingLimited)))
    (return (Variables|Default|GetLatestTiltX))
    (else
      (bind _output_get (Variables|Default|SetLatestTiltX (.roll (Math|Rotator|MakeRotator (* (/ (- (Variables|Default|GetCurrentTiltX) (.x (Variables|Default|GetScreenCenterPivot))) (.x (Variables|Default|GetScreenCenterPivot))) (Variables|Default|GetLimitedRange)) 0.0 0.0))))
      (return _output_get))))

(fn TiltAxisY
  (if (or (>= (Variables|Default|GetCurrentTiltY) (- (.y (Viewport|GetViewportSize)) (Variables|Default|GetPaddingLimited))) (<= (Variables|Default|GetCurrentTiltY) (Variables|Default|GetPaddingLimited)))
    (return (Variables|Default|GetLatestTiltY))
    (else
      (bind _output_get (Variables|Default|SetLatestTiltY (.pitch (Math|Rotator|MakeRotator 0.0 (* (/ (- (Variables|Default|GetCurrentTiltY) (.y (Variables|Default|GetScreenCenterPivot))) (.y (Variables|Default|GetScreenCenterPivot))) (Variables|Default|GetLimitedRange)) 0.0))))
      (return _output_get))))