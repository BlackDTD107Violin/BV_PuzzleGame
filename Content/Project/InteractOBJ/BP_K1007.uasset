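; BP_K1007 is an inspectable key item with a chalice material that can be picked up and used in a keyhole.
; Inspector events play a sound, hide it and release it from any extraction target it occupies.
; An animation switcher routes to the keyhole rotation event, which optionally detaches it from the player and destroys it.
; A dynamic material fades an extraction glow in or out using delta time.
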(event Custom|AnimPlay_RotateInKeyHole
  (Development|PrintString "PlayK1001Anim")
  (if (Variables|Default|GetDelete%20if%20Complete) ; Detect destroy or not when animation Complete
    (Default|OBJDetach (Variables|Default|GetPlayer))
    (Actor|DestroyActor)
    (else
      (Development|PrintString "Still in Map and Can Interact"))))

(event EventBeginPlay
  (|CallParentFunction)
  (bind _asbp_first_person_character (Utilities|Casting|CastToBP_FirstPersonCharacter (Game|GetPlayerCharacter 0)))
  (Variables|Default|SetPlayer _asbp_first_person_character)
  (bind _returnvalue (Rendering|Material|CreateDynamicMaterialInstance (Variables|Default|GetStaticMesh) 0 "/Game/Project/AncientTreasures/Materials/Instances/MI_Chalice_01.MI_Chalice_01" "None" :!class /Script/Engine.PrimitiveComponent))
  (Utilities|Array|Add (Variables|Default|GetExtractMatgroups) _returnvalue))

(event EventAnimPlaySwitcher
  (params (bDeleteIfComplete :type Boolean) (AnimTarget :type Name :default "None"))
  (Variables|Default|SetDelete%20if%20Complete bDeleteIfComplete)
  (switch name AnimTarget
    (:RotateInKeyHole
      (CallFunction|AnimPlayRotateinKeyHole))))

(event EventEnterInspector
  (Audio|SpawnSoundAttached (Variables|Default|GetInteractSE) (Variables|Default|GetStaticMesh) "None" "0, 0, 0" "0, 0, 0" "KeepRelativeOffset" false 1.0 1.0 0.0 0 0)
  (Development|SetHiddeninGame (Variables|Default|GetStaticMesh) true false)
  (Utilities|IsValid (Variables|Default|GetCurrentInsertedExtractTA)
    (:Is%20Valid
      (Default|PickOutOBJ (Variables|Default|GetCurrentInsertedExtractTA)))))

(event EventExitInspector
  (Audio|SpawnSoundAttached (Variables|Default|GetInteractSE) (Variables|Default|GetStaticMesh) "None" "0, 0, 0" "0, 0, 0" "KeepRelativeOffset" false 1.0 1.0 0.0 0 0)
  (Rendering|SetActorHiddenInGame true)
  (Collision|SetActorEnableCollision false))

(event EventOBJExtractGlowing
  (params (bIsExtracting :type Boolean))
  (if bIsExtracting
    (if (< (Variables|Default|GetExtractLerpAlpha) 1.0)
      (bind _output_get (Variables|Default|SetExtractLerpAlpha (+ (Variables|Default|GetExtractLerpAlpha) (Utilities|Time|GetWorldDeltaSeconds))))
      (CallFunction|SetExtractMatVal _output_get))
    (elif (> (Variables|Default|GetExtractLerpAlpha) 0.0)
      (bind _output_get_2 (Variables|Default|SetExtractLerpAlpha (- (Variables|Default|GetExtractLerpAlpha) (Utilities|Time|GetWorldDeltaSeconds))))
      (CallFunction|SetExtractMatVal _output_get_2))))

(fn ConstructionScript
  (|CallParentFunction))