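; Tilt-board magnet interactable where the mouse tilts a plate and slides a magnet to capture a pickup.
; Each tick, cursor offset from screen center becomes a range-scaled tilt, holding its last value inside the screen-edge padding.
; The plate lerps toward that tilt while the magnet lerps along it, clamped to borders.
; The child BP_MagnetPickups receives magnet references on BeginPlay and is captured upon overlapping MagneticTA.
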(event OnComponentBeginOverlap(MagneticTA)
  (params (OverlappedComponent :type Primitive%20Component%20Object%20Reference) (OtherActor :type Actor%20Object%20Reference) (OtherComp :type Primitive%20Component%20Object%20Reference) (OtherBodyIndex :type Integer) (bFromSweep :type Boolean) (SweepResult :type Hit%20Result%20Structure%20%28by%20ref%29))
  (bind _asbp_magnet_pickups (Utilities|Casting|CastToBP_MagnetPickups (Variables|/Script/Engine.ChildActorComponent|GetChildActor (Variables|Default|GetMagnetTarget))))
  (if (== _asbp_magnet_pickups OtherActor)
    (Default|CapturedbyMagnet _asbp_magnet_pickups)))

(event EventBeginPlay
  (bind _returnvalue (Viewport|GetViewportSize))
  (|CallParentFunction)
  (Variables|Default|SetScreenCenterPivot (Math|Vector2D|MakeVector2D (/ (.x _returnvalue) 2.0) (/ (.y _returnvalue) 2.0)))
  (bind _asbp_magnet_pickups (Utilities|Casting|CastToBP_MagnetPickups (Variables|/Script/Engine.ChildActorComponent|GetChildActor (Variables|Default|GetMagnetTarget))))
  (Variables|/Game/Project/InteractOBJ/BP_MagnetPickups.BP_MagnetPickups_C|SetMagnetTACone _asbp_magnet_pickups (Variables|Default|GetMagneticTA))
  (Variables|/Game/Project/InteractOBJ/BP_MagnetPickups.BP_MagnetPickups_C|SetMagnetHook _asbp_magnet_pickups (Variables|Default|GetMagnet)))

(event EventTick
  (params (DeltaSeconds :type Float%20%28single-precision%29))
  (CallFunction|TiltDetect))

(fn ConstructionScript
  (|CallParentFunction))

(fn TiltDetect
  (Utilities|FlowControl|Sequence
    (:then_0
      (CallFunction|UpdateCurrentTiltXY)
      (bind _tiltx (CallFunction|TiltAxisX))
      (LocalVariables|SetTiltX _tiltx)
      (bind _tilty (CallFunction|TiltAxisY))
      (LocalVariables|SetTiltY _tilty))
    (:then_1
      (Transformation|SetRelativeRotation (Variables|Default|GetBasePlate) (Math|Rotator|Lerp(Rotator) (Variables|/Script/Engine.SceneComponent|GetRelativeRotation (Variables|Default|GetBasePlate)) (Math|Rotator|MakeRotator (+ (LocalVariables|GetTiltX) 9e+01) (LocalVariables|GetTiltY) 0.0) 0.1 true) false false))
    (:then_2
      (bind _targetpos (CallFunction|CheckMagnetIsTouchBorder (LocalVariables|GetTiltX) (LocalVariables|GetTiltY)))
      (Transformation|SetRelativeLocation (Variables|Default|GetMagnetBase) (Math|Vector|Lerp(Vector) (Variables|/Script/Engine.SceneComponent|GetRelativeLocation (Variables|Default|GetMagnetBase)) _targetpos 0.1) false false))))

(fn TiltAxisX
  (if (or (>= (Variables|Default|GetCurrentTiltX) (- (.x (Viewport|GetViewportSize)) (Variables|Default|GetPaddingLimited))) (<= (Variables|Default|GetCurrentTiltX) (Variables|Default|GetPaddingLimited)))
    (return (Variables|Default|GetLatestTiltX))
    (else
      (bind _output_get (Variables|Default|SetLatestTiltX (.roll (Math|Rotator|MakeRotator (* (/ (- (Variables|Default|GetCurrentTiltX) (.x (Variables|Default|GetScreenCenterPivot))) (.x (Variables|Default|GetScreenCenterPivot))) (Variables|Default|GetLimitedRange)) 0.0 0.0))))
      (return _output_get))))

(fn TiltAxisY
  (if (or (>= (Variables|Default|GetCurrentTiltY) (- (.y (Viewport|GetViewportSize)) (Variables|Default|GetPaddingLimited))) (<= (Variables|Default|GetCurrentTiltY) (Variables|Default|GetPaddingLimited)))
    (return (Variables|Default|GetLatestTiltY))
    (else
      (bind _output_get (Variables|Default|SetLatestTiltY (.pitch (Math|Rotator|MakeRotator 0.0 (* (/ (- (Variables|Default|GetCurrentTiltY) (.y (Variables|Default|GetScreenCenterPivot))) (.y (Variables|Default|GetScreenCenterPivot))) (Variables|Default|GetLimitedRange)) 0.0))))
      (return _output_get))))

(fn UpdateCurrentTiltXY
  (bind _returnvalue (Game|GetPlayerController 0))
  (bind _worldlocation (Game|Player|ConvertMouseLocationToWorldSpace _returnvalue))
  (bind _screenlocation (Class|PlayerController|ProjectWorldLocationtoScreen _returnvalue _worldlocation false))
  (Variables|Default|SetCurrentTiltX (.x _screenlocation))
  (Variables|Default|SetCurrentTiltY (.y _screenlocation)))

(fn CheckMagnetIsTouchBorder
  (params (InputX :type Float%20%28double-precision%29) (InputY :type Float%20%28double-precision%29))
  (bind _magnetbase (Variables|Default|GetMagnetBase))
  (bind _relativelocation (Variables|/Script/Engine.SceneComponent|GetRelativeLocation _magnetbase))
  (Variables|Default|SetAssumeTargetPosa (Math|Vector|MakeVector (- (.x _relativelocation) InputY) (+ InputX (.y _relativelocation)) (.z _relativelocation)))
  (CallFunction|CheckBorderX)
  (CallFunction|CheckBorderY)
  (return (Variables|Default|GetAssumeTargetPosa)))

(fn CheckBorderX
  (if (>= (.x (Variables|Default|GetAssumeTargetPosa)) (Variables|Default|GetMaxBorder_X))
    (Variables|Default|SetAssumeTargetPosa (Math|Vector|MakeVector (Variables|Default|GetMaxBorder_X) (.y (Variables|Default|GetAssumeTargetPosa)) (.z (Variables|Default|GetAssumeTargetPosa))))
    (elif (<= (.x (Variables|Default|GetAssumeTargetPosa)) (Variables|Default|GetMinBorder_X))
      (Variables|Default|SetAssumeTargetPosa (Math|Vector|MakeVector (Variables|Default|GetMinBorder_X) (.y (Variables|Default|GetAssumeTargetPosa)) (.z (Variables|Default|GetAssumeTargetPosa)))))))

(fn CheckBorderY
  (if (>= (.y (Variables|Default|GetAssumeTargetPosa)) (Variables|Default|GetMaxBorder_Y))
    (Variables|Default|SetAssumeTargetPosa (Math|Vector|MakeVector (.x (Variables|Default|GetAssumeTargetPosa)) (Variables|Default|GetMaxBorder_Y) (.z (Variables|Default|GetAssumeTargetPosa))))
    (elif (<= (.y (Variables|Default|GetAssumeTargetPosa)) (Variables|Default|GetMinBorder_Y))
      (Variables|Default|SetAssumeTargetPosa (Math|Vector|MakeVector (.x (Variables|Default|GetAssumeTargetPosa)) (Variables|Default|GetMinBorder_Y) (.z (Variables|Default|GetAssumeTargetPosa)))))))