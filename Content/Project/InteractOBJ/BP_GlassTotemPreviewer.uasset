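; BP_GlassTotemPreviewer previews a glass totem pattern from its texture or spline shape and distance, expand, rotate and scale codes.
; Original mode drives a dynamic material on a plane, either one totem (BASE) or indexed slots tracked per side (UNITE).
; Spline mode hides the plane and arranges up to six child-actor BP_CoreSplines radially through their pivots.
; Separate functions clear the preview or update its codes live.
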(event EventBeginPlay
  (switch Utilities|FlowControl|Switch|SwitchonE_GLASSType (Variables|Default|GetPreviewerType)
    (:NewEnumerator6
      (bind _returnvalue (Rendering|Material|CreateDynamicMaterialInstance (Variables|Default|GetPlane) 0 "/Game/Project/MaterialLibrary/M_GlassTotem_Inst.M_GlassTotem_Inst" "None" :!class /Script/Engine.PrimitiveComponent))
      (Variables|Default|SetMat_GlassTotem _returnvalue))
    (:NewEnumerator1
      (bind _returnvalue_2 (Rendering|Material|CreateDynamicMaterialInstance (Variables|Default|GetPlane) 0 "/Game/Project/MaterialLibrary/M_GlassUniteTotem_Inst.M_GlassUniteTotem_Inst" "None" :!class /Script/Engine.PrimitiveComponent))
      (Variables|Default|SetMat_GlassUniteTotem _returnvalue_2)))
  (Utilities|Array|Add (Variables|Default|GetSplineGroup) (Variables|Default|GetSpline_1))
  (Utilities|Array|Add (Variables|Default|GetSplineGroup) (Variables|Default|GetSpline_2))
  (Utilities|Array|Add (Variables|Default|GetSplineGroup) (Variables|Default|GetSpline_3))
  (Utilities|Array|Add (Variables|Default|GetSplineGroup) (Variables|Default|GetSpline_4))
  (Utilities|Array|Add (Variables|Default|GetSplineGroup) (Variables|Default|GetSpline_5))
  (Utilities|Array|Add (Variables|Default|GetSplineGroup) (Variables|Default|GetSpline_6)))

(fn ConstructionScript
  (|CallParentFunction))

(fn ClearPreviewer
  (params (Side :type E_SideState%20Enum :default "NewEnumerator0"))
  (bind _mat_glasstotem (Variables|Default|GetMat_GlassTotem))
  (LocalVariables|SetL_NotchSide Side)
  (switch Utilities|FlowControl|Switch|SwitchonE_TotemPreview (Variables|Default|GetTotemPreviewType)
    (:NewEnumerator0
      (switch Utilities|FlowControl|Switch|SwitchonE_GLASSType (Variables|Default|GetPreviewerType)
        (:NewEnumerator6
          (Rendering|Material|SetScalarParameterValue _mat_glasstotem "Input_Distance" 3.0 :!class /Script/Engine.MaterialInstanceDynamic)
          (Rendering|Material|SetScalarParameterValue _mat_glasstotem "Input_Expand" 0.0 :!class /Script/Engine.MaterialInstanceDynamic)
          (Rendering|Material|SetScalarParameterValue _mat_glasstotem "Input_Rotate" 0.0 :!class /Script/Engine.MaterialInstanceDynamic)
          (Rendering|Material|SetScalarParameterValue _mat_glasstotem "Input_Scaling" 3.0 :!class /Script/Engine.MaterialInstanceDynamic))
        (:NewEnumerator1
          (CallFunction|EraseValueGLASSUnite (LocalVariables|GetL_NotchSide)))))
    (:NewEnumerator3
      (for _array_element (Variables|Default|GetSplineGroup)
        (ChildActorComponent|SetChildActorClass _array_element 0)))))

(fn ReceiveGLASSPreviewer
  (params (CurrentGLASSBase :type ST%20Glass%20Base%20Collection%20Structure) (ValueSide :type E_SideState%20Enum :default "NewEnumerator0") (CurrentGlassValue :type ST%20Glass%20Value%20Structure))
  (Variables|Default|SetCurrentActivateSide ValueSide)
  (LocalVariables|SetL_CurrentGLASS CurrentGLASSBase)
  (LocalVariables|SetL_CurrentGLASSValue CurrentGlassValue)
  (switch Utilities|FlowControl|Switch|SwitchonE_TotemPreview (Variables|Default|GetTotemPreviewType)
    (:NewEnumerator0
      (switch Utilities|FlowControl|Switch|SwitchonE_GLASSType (Variables|Default|GetPreviewerType)
        (:NewEnumerator6
          (CallFunction|SetupPreviewerGLASSBase (LocalVariables|GetL_CurrentGLASS)))
        (:NewEnumerator1
          (CallFunction|SetupPreviewerGLASSUnite (LocalVariables|GetL_CurrentGLASS)))))
    (:NewEnumerator3
      (CallFunction|SetupPreviewerGLASSSpline (LocalVariables|GetL_CurrentGLASSValue)))))

(fn SetupPreviewerGLASSBase
  (params (ST_GlassBaseCollection :type ST%20Glass%20Base%20Collection%20Structure%20%28by%20ref%29))
  (bind _glassvalue (Utilities|Struct|BreakST_GlassBaseCollection ST_GlassBaseCollection))
  (bind _mat_glasstotem (Variables|Default|GetMat_GlassTotem))
  (bind _output (Utilities|Array|Get(acopy) _glassvalue))
  (bind (_basetotem _code_rotate _code_expand _code_distance _code_scale) (Utilities|Struct|BreakST_GlassValue _output))
  (Rendering|Material|SetTextureParameterValue _mat_glasstotem "MainTotem" _basetotem)
  (Rendering|Material|SetScalarParameterValue _mat_glasstotem "Input_Distance" (Math|Conversions|ToFloat(Integer) _code_distance) :!class /Script/Engine.MaterialInstanceDynamic)
  (Rendering|Material|SetScalarParameterValue _mat_glasstotem "Input_Expand" (Math|Conversions|ToFloat(Integer) _code_expand) :!class /Script/Engine.MaterialInstanceDynamic)
  (Rendering|Material|SetScalarParameterValue _mat_glasstotem "Input_Rotate" (Math|Conversions|ToFloat(Integer) _code_rotate) :!class /Script/Engine.MaterialInstanceDynamic)
  (Rendering|Material|SetScalarParameterValue _mat_glasstotem "Input_Scaling" (Math|Conversions|ToFloat(Integer) _code_scale) :!class /Script/Engine.MaterialInstanceDynamic))

(fn SetupPreviewerGLASSUnite
  (params (ST_GlassBaseCollection :type ST%20Glass%20Base%20Collection%20Structure%20%28by%20ref%29))
  (bind _output_get (LocalVariables|SetL_InsertedGlass ST_GlassBaseCollection))
  (LocalVariables|SetL_GlassValueCount (Utilities|Array|Length (Utilities|Struct|BreakST_GlassBaseCollection _output_get)))
  (bind (_array_element _array_index) (Utilities|Array|ForEachLoopwithBreak (Variables|Default|GetValueSide) :!label _label)
    (:LoopBody
      (LocalVariables|SetL_ArrayIndex (Utilities|String|ToString(Integer) _array_index))
      (if (Utilities|Enum|Equal(Enum) _array_element "NewEnumerator0")
        (|SetBy-RefVar (Utilities|Array|Get(acopy) (Variables|Default|GetValueSide) _array_index) (Variables|Default|GetCurrentActivateSide))
        (Rendering|Material|SetTextureParameterValue (Variables|Default|GetMat_GlassUniteTotem) (Utilities|String|StringToName (Utilities|String|Append (LocalVariables|GetL_MainTotem) (LocalVariables|GetL_ArrayIndex))) (.BaseTotem (Utilities|Struct|BreakST_GlassValue (Utilities|Array|Get(acopy) (Utilities|Struct|BreakST_GlassBaseCollection (LocalVariables|GetL_InsertedGlass)) (LocalVariables|GetL_AssignCount)))))
        (Rendering|Material|SetScalarParameterValue (Variables|Default|GetMat_GlassUniteTotem) (Utilities|String|StringToName (Utilities|String|Append (LocalVariables|GetL_Input_Rotate) (LocalVariables|GetL_ArrayIndex))) (Math|Conversions|ToFloat(Integer) (.Code_Rotate (Utilities|Struct|BreakST_GlassValue (Utilities|Array|Get(acopy) (Utilities|Struct|BreakST_GlassBaseCollection (LocalVariables|GetL_InsertedGlass)) (LocalVariables|GetL_AssignCount))))) :!class /Script/Engine.MaterialInstanceDynamic)
        (Rendering|Material|SetScalarParameterValue (Variables|Default|GetMat_GlassUniteTotem) (Utilities|String|StringToName (Utilities|String|Append (LocalVariables|GetL_Input_Expand) (LocalVariables|GetL_ArrayIndex))) (Math|Conversions|ToFloat(Integer) (.Code_Expand (Utilities|Struct|BreakST_GlassValue (Utilities|Array|Get(acopy) (Utilities|Struct|BreakST_GlassBaseCollection (LocalVariables|GetL_InsertedGlass)) (LocalVariables|GetL_AssignCount))))) :!class /Script/Engine.MaterialInstanceDynamic)
        (Rendering|Material|SetScalarParameterValue (Variables|Default|GetMat_GlassUniteTotem) (Utilities|String|StringToName (Utilities|String|Append (LocalVariables|GetL_Input_Distance) (LocalVariables|GetL_ArrayIndex))) (Math|Conversions|ToFloat(Integer) (.Code_Distance (Utilities|Struct|BreakST_GlassValue (Utilities|Array|Get(acopy) (Utilities|Struct|BreakST_GlassBaseCollection (LocalVariables|GetL_InsertedGlass)) (LocalVariables|GetL_AssignCount))))) :!class /Script/Engine.MaterialInstanceDynamic)
        (Rendering|Material|SetScalarParameterValue (Variables|Default|GetMat_GlassUniteTotem) (Utilities|String|StringToName (Utilities|String|Append (LocalVariables|GetL_Input_Scale) (LocalVariables|GetL_ArrayIndex))) (Math|Conversions|ToFloat(Integer) (.Code_Scale (Utilities|Struct|BreakST_GlassValue (Utilities|Array|Get(acopy) (Utilities|Struct|BreakST_GlassBaseCollection (LocalVariables|GetL_InsertedGlass)) (LocalVariables|GetL_AssignCount))))) :!class /Script/Engine.MaterialInstanceDynamic)
        (LocalVariables|SetL_AssignCount (+ (LocalVariables|GetL_AssignCount) 1))
        (if (== (LocalVariables|GetL_AssignCount) (LocalVariables|GetL_GlassValueCount))
          (goto _label Break))))))

(fn EraseValueGLASSUnite
  (params (Side :type E_SideState%20Enum :default "NewEnumerator0"))
  (LocalVariables|SetL_EraseSide Side)
  (for (_array_element _array_index) (Variables|Default|GetValueSide)
    (LocalVariables|SetL_ArrayIndex _array_index)
    (if (Utilities|Enum|Equal(Enum) _array_element (LocalVariables|GetL_EraseSide))
      (Rendering|Material|SetScalarParameterValue (Variables|Default|GetMat_GlassUniteTotem) (Utilities|String|StringToName (Utilities|String|Append (LocalVariables|GetL_Input_Expand) (Utilities|String|ToString(Integer) (LocalVariables|GetL_ArrayIndex)))) 0.0 :!class /Script/Engine.MaterialInstanceDynamic)
      (|SetBy-RefVar (Utilities|Array|Get(acopy) (Variables|Default|GetValueSide) (LocalVariables|GetL_ArrayIndex)) "NewEnumerator0"))))

(fn SetupPreviewerGLASSSpline
  (params (ST_GlassValue :type ST%20Glass%20Value%20Structure))
  (bind (_splinetotem _code_rotate _code_expand _code_distance _code_scale) (Utilities|Struct|BreakST_GlassValue ST_GlassValue))
  (Rendering|SetVisibility (Variables|Default|GetPlane) false false)
  (Variables|Default|SetExpandCount _code_expand)
  (for (_array_element _array_index) (Variables|Default|GetSplineGroup)
    (Rendering|SetVisibility _array_element (< _array_index (Variables|Default|GetExpandCount)) false)
    (ChildActorComponent|SetChildActorClass _array_element _splinetotem))
  (CallFunction|SplineDistance _code_distance)
  (CallFunction|SplineExpand)
  (CallFunction|SplineRotate _code_rotate)
  (CallFunction|SplineScale _code_scale))

(fn SplineExpand
  (for (_array_element _array_index) (Variables|Default|GetSplineGroup)
    (if (< _array_index (Variables|Default|GetExpandCount))
      (bind _asbp_core_spline (Utilities|Casting|CastToBP_CoreSpline (Variables|/Script/Engine.ChildActorComponent|GetChildActor _array_element)))
      (Transformation|SetRelativeRotation (Variables|/Game/Project/Core/GlassCollection/BP_CoreSpline.BP_CoreSpline_C|GetMainPivot _asbp_core_spline) (Math|Rotator|MakeRotator 0.0 (Math|Conversions|ToFloat(Integer) (* _array_index (/ 360 (Variables|Default|GetExpandCount)))) 0.0) false false))))

(fn SplineRotate
  (params (RotateValue :type Integer))
  (LocalVariables|SetL_value RotateValue)
  (for (_array_element _array_index) (Variables|Default|GetSplineGroup)
    (if (< _array_index (Variables|Default|GetExpandCount))
      (bind _asbp_core_spline (Utilities|Casting|CastToBP_CoreSpline (Variables|/Script/Engine.ChildActorComponent|GetChildActor _array_element)))
      (Transformation|SetRelativeRotation (Variables|/Game/Project/Core/GlassCollection/BP_CoreSpline.BP_CoreSpline_C|GetChildPivot _asbp_core_spline) (Math|Rotator|MakeRotator 0.0 (Math|Conversions|ToFloat(Integer) (* (LocalVariables|GetL_value) 60)) 0.0) false false))))

(fn SplineDistance
  (params (DistanceValue :type Integer))
  (LocalVariables|SetL_value DistanceValue)
  (for (_array_element _array_index) (Variables|Default|GetSplineGroup)
    (if (< _array_index (Variables|Default|GetExpandCount))
      (bind _asbp_core_spline (Utilities|Casting|CastToBP_CoreSpline (Variables|/Script/Engine.ChildActorComponent|GetChildActor _array_element)))
      (Transformation|SetRelativeLocation (Variables|/Game/Project/Core/GlassCollection/BP_CoreSpline.BP_CoreSpline_C|GetChildPivot _asbp_core_spline) (Math|Vector|MakeVector 0.0 0.0 (Math|Conversions|ToFloat(Integer) (* (LocalVariables|GetL_value) 10))) false false))))

(fn SplineScale
  (params (ScaleValue :type Integer))
  (LocalVariables|SetL_value ScaleValue)
  (for (_array_element _array_index) (Variables|Default|GetSplineGroup)
    (if (< _array_index (Variables|Default|GetExpandCount))
      (bind _asbp_core_spline (Utilities|Casting|CastToBP_CoreSpline (Variables|/Script/Engine.ChildActorComponent|GetChildActor _array_element)))
      (Transformation|SetRelativeScale3D (Variables|/Game/Project/Core/GlassCollection/BP_CoreSpline.BP_CoreSpline_C|GetChildPivot _asbp_core_spline) (Math|Vector|MakeVector (+ (* (Math|Conversions|ToFloat(Integer) (LocalVariables|GetL_value)) 0.2) 0.2) (.y (Variables|/Script/Engine.SceneComponent|GetRelativeScale3D (Variables|/Game/Project/Core/GlassCollection/BP_CoreSpline.BP_CoreSpline_C|GetChildPivot _asbp_core_spline))) (+ (* (Math|Conversions|ToFloat(Integer) (LocalVariables|GetL_value)) 0.2) 0.2))))))

(fn UpdatePreviewerGLASSSpline
  (params (Distance :type Integer) (Expand :type Integer) (Rotate :type Integer) (Scaling :type Integer))
  (LocalVariables|SetL_DistanceUpdate Distance)
  (bind _output_get (Variables|Default|SetExpandCount Expand))
  (Math|Integer|IncrementInt _output_get
    (:%20%20
      (LocalVariables|SetL_RotateUpdate Rotate)
      (LocalVariables|SetL_ScaleUpdate Scaling)
      (if (Utilities|Enum|Equal(Enum) (Variables|Default|GetTotemPreviewType) "NewEnumerator0")
        (Rendering|Material|SetScalarParameterValue (Variables|Default|GetMat_GlassTotem) "Input_Distance" (Math|Conversions|ToFloat(Integer) (LocalVariables|GetL_DistanceUpdate)) :!class /Script/Engine.MaterialInstanceDynamic)
        (Rendering|Material|SetScalarParameterValue (Variables|Default|GetMat_GlassTotem) "Input_Expand" (Math|Conversions|ToFloat(Integer) (Variables|Default|GetExpandCount)) :!class /Script/Engine.MaterialInstanceDynamic)
        (Rendering|Material|SetScalarParameterValue (Variables|Default|GetMat_GlassTotem) "Input_Rotate" (Math|Conversions|ToFloat(Integer) (LocalVariables|GetL_RotateUpdate)) :!class /Script/Engine.MaterialInstanceDynamic)
        (Rendering|Material|SetScalarParameterValue (Variables|Default|GetMat_GlassTotem) "Input_Scaling" (Math|Conversions|ToFloat(Integer) (LocalVariables|GetL_ScaleUpdate)) :!class /Script/Engine.MaterialInstanceDynamic)
        (else
          (for (_array_element _array_index) (Variables|Default|GetSplineGroup)
            (Rendering|SetVisibility _array_element (< _array_index (Variables|Default|GetExpandCount)) false))
          (CallFunction|SplineDistance (LocalVariables|GetL_DistanceUpdate))
          (CallFunction|SplineExpand)
          (CallFunction|SplineRotate (LocalVariables|GetL_RotateUpdate))
          (CallFunction|SplineScale (LocalVariables|GetL_ScaleUpdate)))))))