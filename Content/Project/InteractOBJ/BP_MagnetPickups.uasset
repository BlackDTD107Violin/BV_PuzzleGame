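; BP_MagnetPickups is an interactable pickup that gets pulled in and held by a magnet.
; CapturedByMagnet plays a timeline that interpolates the actor toward MagnetHook, adding the timeline track to the interpolated position.
; When its mesh overlaps MagnetTACone it is flagged as captured, and Tick then snaps it to that component's location every frame with no sweep.
; Nothing in this graph clears the captured flag.
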(event OnComponentBeginOverlap(StaticMesh)
  (params (OverlappedComponent :type Primitive%20Component%20Object%20Reference) (OtherActor :type Actor%20Object%20Reference) (OtherComp :type Primitive%20Component%20Object%20Reference) (OtherBodyIndex :type Integer) (bFromSweep :type Boolean) (SweepResult :type Hit%20Result%20Structure%20%28by%20ref%29))
  (if (== OtherComp (Variables|Default|GetMagnetTACone))
    (Variables|Default|SetbIsAlreadyCaptured true)))

(event Custom|CapturedByMagnet
  (if (not (Variables|Default|GetbIsAlreadyCaptured))
    (bind _newtrack_0 (Timeline|Timeline PlayFromStart)
      (:Update
        (Transformation|SetActorLocation (+ _newtrack_0 (Math|Interpolation|VInterpTo (.Location (Math|Transform|BreakTransform (Transformation|GetActorTransform))) (Transformation|GetWorldLocation (Variables|Default|GetMagnetHook)) (Utilities|Time|GetWorldDeltaSeconds) 2.0)) false false)))))

(event EventTick
  (params (DeltaSeconds :type Float%20%28single-precision%29))
  (if (Variables|Default|GetbIsAlreadyCaptured)
    (Transformation|SetActorLocation (Transformation|GetWorldLocation (Variables|Default|GetMagnetTACone)) false false)))

(fn ConstructionScript
  (|CallParentFunction))