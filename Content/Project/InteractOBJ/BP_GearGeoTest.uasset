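; BP_GearGeoTest is a test actor, apparently for a gear, that exercises Geometry Cache playback through keyboard input enabled on BeginPlay.
; T toggles running, Y switches between forward and reversed play, and U and I raise or lower playback speed.
; O advances the start time offset, wrapping it at the cache duration.
; A debug print of frame count, time and duration is left unconnected.
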(event EventBeginPlay
  (Input|EnableInput (Game|GetPlayerController 0)))

(event EventTick
  (params (DeltaSeconds :type Float%20%28single-precision%29)))

(event Input|KeyboardEvents|T
  (params (Key :type Key%20Structure :default "None"))
  (:Pressed
    (bind _output_get (Variables|Default|SetbIsRunning (not (Variables|Default|GetbIsRunning))))
    (Variables|/Script/GeometryCache.GeometryCacheComponent|SetbRunning (Variables|Default|GetGeometryCacheComponent) _output_get)))

(event Input|KeyboardEvents|Y
  (params (Key :type Key%20Structure :default "None"))
  (:Pressed
    (bind _output_get (Variables|Default|SetbIsFoward (not (Variables|Default|GetbIsFoward))))
    (if _output_get
      (Audio|Components|Audio|Play (Variables|Default|GetGeometryCacheComponent))
      (else
        (Class|GeometryCacheComponent|PlayReversed (Variables|Default|GetGeometryCacheComponent))))))

(event Input|KeyboardEvents|U
  (params (Key :type Key%20Structure :default "None"))
  (:Pressed
    (bind _output_get (Variables|Default|SetSpeed (+ (Variables|Default|GetSpeed) 1.0)))
    (Class|GeometryCacheComponent|SetPlaybackSpeed (Variables|Default|GetGeometryCacheComponent) _output_get)))

(event Input|KeyboardEvents|I
  (params (Key :type Key%20Structure :default "None"))
  (:Pressed
    (if (>= (Variables|Default|GetSpeed) 1.0)
      (bind _output_get (Variables|Default|SetSpeed (+ (Variables|Default|GetSpeed) -1.0)))
      (Class|GeometryCacheComponent|SetPlaybackSpeed (Variables|Default|GetGeometryCacheComponent) _output_get))))

(event Input|KeyboardEvents|O
  (params (Key :type Key%20Structure :default "None"))
  (:Pressed
    (bind _output_get (Variables|Default|SetStartTime (+ (Variables|Default|GetStartTime) 1.0)))
    (if (>= _output_get (Variables|/Script/GeometryCache.GeometryCacheComponent|GetDuration (Variables|Default|GetGeometryCacheComponent)))
      (bind _output_get_2 (Variables|Default|SetStartTime (- (Variables|Default|GetStartTime) (Variables|/Script/GeometryCache.GeometryCacheComponent|GetDuration (Variables|Default|GetGeometryCacheComponent)))))
      (Class|GeometryCacheComponent|SetStartTimeOffset (Variables|Default|GetGeometryCacheComponent) _output_get_2)
      (else
        (Class|GeometryCacheComponent|SetStartTimeOffset (Variables|Default|GetGeometryCacheComponent) (Variables|Default|GetStartTime))))))

(fn ConstructionScript)