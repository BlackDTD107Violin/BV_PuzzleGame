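; BP_R0001 is an interactable READ object with serial R0001, tied to the tutorial first-person character.
; AttachtoHand notifies the player with the serial, plays the object's sound and returns CurrentAttachSET when valid.
; Repos restores the original transform and sound; if parented, it reattaches at the serial-named socket on the root cached by SetTempPos, notifies the player and triggers a one-time tutorial arrival that clears the prompt UI.
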(event EventBeginPlay
  (|CallParentFunction)
  (Variables|Default|SetREADSerialCode "R0001")
  (bind _asbp_first_person_character_tutorial (Utilities|Casting|CastToBP_FirstPersonCharacterTutorial (Game|GetPlayerCharacter 0)))
  (Variables|Default|SetPlayer _asbp_first_person_character_tutorial))

(event EventSetTempPos
  (params (Root :type Static%20Mesh%20Component%20Object%20Reference))
  ;[0.05098 0.05098 0.05098] Temp Repos will execute when the root parent is moving
  (Variables|Default|SetReAttach Root))

(event EventRepos
  (Transformation|SetActorRelativeTransform (Variables|Default|GetOriginalPos) false false)
  (Audio|SpawnSoundAttached "/Game/Project/Audio/MetaSoundSource/MSS_R0001.MSS_R0001" (Variables|Default|GetStaticMesh) "None" "0, 0, 0" "0, 0, 0" "KeepRelativeOffset" false 1.0 1.0 0.0 0 0)
  (if (Variables|Default|GetbHasParent)
    (Transformation|AttachComponentToComponent (Variables|Default|GetReAttach) (Variables|Default|GetREADSerialCode) "SnapToTarget" "KeepWorld" "KeepWorld" true)
    (Default|InteractwithREAD (Variables|Default|GetPlayer) (Variables|Default|GetREADSerialCode))
    (if (not (Variables|Default|GetbHasTriggerTutor))
      (Variables|Default|SetbHasTriggerTutor true)
      (Default|ArriveTutorialTA (Variables|Default|GetPlayer))
      (Default|ClearGamePromptUIView (Variables|Default|GetPlayer)))))

(fn ConstructionScript
  (|CallParentFunction))

(fn AttachtoHand
  (params (InteractTarget :type Actor%20Component%20Object%20Reference))
  (Default|InteractwithREAD (Variables|Default|GetPlayer) (Variables|Default|GetREADSerialCode))
  (Audio|SpawnSoundAttached "/Game/Project/Audio/MetaSoundSource/MSS_R0001.MSS_R0001" (Variables|Default|GetStaticMesh) "None" "0, 0, 0" "0, 0, 0" "KeepRelativeOffset" false 1.0 1.0 0.0 0 0)
  (Utilities|IsValid (Variables|Default|GetCurrentAttachSET)
    (:Is%20Valid
      (return (Variables|Default|GetCurrentAttachSET)))))