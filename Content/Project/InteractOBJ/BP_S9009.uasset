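; BP_S9009 is an interactable puzzle prop where a mixer "CoStarter" handle reveals a final item once an inserted glass's code matches.
; Interacting blends to a zoom camera per trigger and toggles collision on triggers and parts.
; Tick turns vertical mouse drag into clamped handle movement with slide and lock sounds, easing it home or open on release.
; StartCheckMatchCode compares glass totem values against stored codes, unlocking the handle's full travel.
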(event OnClicked(SM_Mixer_Co_Starter_Handle)
  (params (TouchedComponent :type Primitive%20Component%20Object%20Reference) (ButtonPressed :type Key%20Structure :default "None"))
  (Variables|Default|SetbIsDragSlider true)
  (Variables|/Game/ProjectDefault/FirstPerson/Blueprints/BP_FirstPersonCharacter.BP_FirstPersonCharacter_C|SetCurrentInteract (Variables|S9009|GetPlayer) self))

(event Custom|Play%20Film%20Setup
  (Utilities|FlowControl|Sequence
    (:then_0
      (Default|ToggleInputFilm (Variables|S9009|GetPlayer) true false))
    (:then_1
      (Utilities|FlowControl|Delay 1.0))))

(event EventBeginPlay
  (bind _returnvalue (Game|GetPlayerController 0))
  (|CallParentFunction)
  (bind _asbp_first_person_character (Utilities|Casting|CastToBP_FirstPersonCharacter (Game|GetPlayerCharacter 0)))
  (Variables|S9009|SetPlayer _asbp_first_person_character)
  (Input|EnableInput _returnvalue)
  (Variables|/Script/Engine.PlayerController|SetbEnableClickEvents _returnvalue true)
  (Variables|/Script/Engine.PlayerController|SetbEnableMouseOverEvents _returnvalue true)
  (CallFunction|PresetValue))

(event EventInteract
  (params (InteractActor :type Actor%20Object%20Reference) (InteractTarget :type Actor%20Component%20Object%20Reference))
  (CallFunction|Zoomin InteractTarget))

(event EventZoomin
  (params (ZoomComponent :type Actor%20Component%20Object%20Reference))
  (bind _returnvalue (Game|GetPlayerController 0))
  (bind _biszoomset (CallFunction|AssignZoomPosition ZoomComponent))
  (if _biszoomset
    (Game|Player|SetViewTargetwithBlend (Game|GetPlayerController 0) self 0.5 "VTBlend_Linear" 0.0 true)
    (Input|SetIgnoreMoveInput _returnvalue true)
    (Input|SetIgnoreLookInput _returnvalue true)
    (Default|ClearGamePromptUIView (Variables|S9009|GetPlayer))
    (CallFunction|SwitchTACollisionProfile false)))

(event EventTick
  (params (DeltaSeconds :type Float%20%28single-precision%29))
  (if (Variables|Default|GetbIsStandBy)
    (CallFunction|BacktoDefault(Empty))
    (else
      (switch int (Variables|S9009|GetZoomInPart)
        (:0
          (CallFunction|CheckState-CoStarter))))))

(event EventInteractEnd
  (Variables|/Game/ProjectDefault/FirstPerson/Blueprints/BP_FirstPersonCharacter.BP_FirstPersonCharacter_C|SetCurrentInteract (Variables|S9009|GetPlayer) self)
  (Variables|Default|SetbSoundPlaying false)
  (switch int (Variables|S9009|GetZoomInPart)
    (:0
      (Variables|Default|SetbIsDragSlider false))))

(event EventZoomOut
  (bind _returnvalue (Game|GetPlayerController 0))
  (Game|Player|SetViewTargetwithBlend (Game|GetPlayerController 0) (Game|GetPlayerCharacter 0) 0.5 "VTBlend_Linear" 0.0 true)
  (CallFunction|SwitchMeshCollisionProfile false)
  (Input|ResetIgnoreMoveInput _returnvalue)
  (Input|ResetIgnoreLookInput _returnvalue)
  (Variables|Default|SetbIsStandBy true)
  (Utilities|FlowControl|Delay 1.0)
  (CallFunction|SwitchTACollisionProfile true))

(fn ConstructionScript
  (|CallParentFunction))

(fn AssignZoomPosition
  (params (ZoomInComponent :type Object%20Object%20Reference))
  (LocalVariables|SetL_FindZoomInPoint false)
  (bind (_array_element _array_index) (Utilities|Array|ForEachLoopwithBreak (Variables|S9009|GetGroupWidgetTrigger) :!label _label)
    (:LoopBody
      (if (== _array_element ZoomInComponent)
        (Variables|S9009|SetZoomInPart _array_index)
        (LocalVariables|SetL_FindZoomInPoint true)
        (goto _label Break)))
    (:Completed
      (if (LocalVariables|GetL_FindZoomInPoint)
        _
        (else
          _))
      (Transformation|SetRelativeTransform (Variables|Default|GetZoomInCamera) (Utilities|Array|Get(acopy) (Variables|S9009|GetZoomInPoint) (Variables|S9009|GetZoomInPart)) false false)
      (CallFunction|SwitchMeshCollisionProfile true)
      (Variables|Default|SetbIsStandBy false)
      (return true))))

(fn BacktoDefault(Empty))

(fn CheckState-CoStarter
  (if (Variables|Default|GetbIsDragSlider)
    (if (Variables|Default|GetbHasUpdateMousePivot)
      (CallFunction|CoStarter-DragViaInput)
      (else
        (Variables|Default|SetbHasUpdateMousePivot true)
        (CallFunction|UpdateTriggerMousePivot)))
    (else
      (Variables|Default|SetbHasUpdateMousePivot false)
      (Variables|Default|SetLatestDir_CoStarter 0)
      (if (and (Variables|Default|GetbFinalItemIsCreate) (<= (.z (Variables|/Script/Engine.SceneComponent|GetRelativeLocation (Variables|Default|GetSM_Mixer_Co_Starter_Handle))) 149.5))
        (CallFunction|CoStarter-FinishRemainOffset true)
        (else
          (CallFunction|CoStarter-FinishRemainOffset false))))))

(fn CoStarter-DragViaInput
  (bind _returnvalue (Game|GetPlayerController 0))
  (bind _triggermousepivot (Variables|S9009|GetTriggerMousePivot))
  (bind _sm_mixer_co_starter_handle (Variables|Default|GetSM_Mixer_Co_Starter_Handle))
  (bind _worldlocation (Game|Player|ConvertMouseLocationToWorldSpace _returnvalue))
  (bind _relativelocation (Variables|/Script/Engine.SceneComponent|GetRelativeLocation _sm_mixer_co_starter_handle))
  (bind _screenlocation (Class|PlayerController|ProjectWorldLocationtoScreen _returnvalue _worldlocation false))
  (if (!= (.y _screenlocation) (.y _triggermousepivot))
    (LocalVariables|SetL_IsFowardDir (> (.y _screenlocation) (.y _triggermousepivot)))
    (Utilities|FlowControl|Sequence
      (:then_0
        (if (LocalVariables|GetL_IsFowardDir)
          (LocalVariables|SetL_SpeedDir -1.0)
          (if (Variables|Default|GetbGlassCodeIsMatch)
            (LocalVariables|SetL_LimitedLocation 144.5)
            (else
              (LocalVariables|SetL_LimitedLocation 192.5)))
          (LocalVariables|SetL_CurrentDir 1)
          (else
            (LocalVariables|SetL_SpeedDir 1.0)
            (LocalVariables|SetL_LimitedLocation 194.5)
            (LocalVariables|SetL_CurrentDir -1)))
        (Variables|Default|SetbSoundPlaying (== (LocalVariables|GetL_CurrentDir) (Variables|Default|GetLatestDir_CoStarter)))
        (Variables|Default|SetLatestDir_CoStarter (LocalVariables|GetL_CurrentDir))
        (Transformation|AddLocalOffset (Variables|Default|GetSM_Mixer_Co_Starter_Handle) (Math|Vector|MakeVector 0.0 0.0 (* (Variables|Default|GetSliderSpeed) (LocalVariables|GetL_SpeedDir))) false false))
      (:then_1
        (if (LocalVariables|GetL_IsFowardDir)
          (if (<= (.z (Variables|/Script/Engine.SceneComponent|GetRelativeLocation (Variables|Default|GetSM_Mixer_Co_Starter_Handle))) (LocalVariables|GetL_LimitedLocation))
            (Transformation|SetRelativeLocation _sm_mixer_co_starter_handle (Math|Vector|MakeVector (.x _relativelocation) (.y _relativelocation) (LocalVariables|GetL_LimitedLocation)) false false :!label _label)
            (Variables|Default|SetbHasUpdateMousePivot false)
            (if (== (LocalVariables|GetL_LimitedLocation) 144.5)
              (CallFunction|CheckCreateFinalItemRequest)
              (Audio|SpawnSoundAttached "/Game/Project/Audio/MetaSoundSource/SE/MSS_Drawer_Slide_1.MSS_Drawer_Slide_1" 0 "None" "0, 0, 0" "0, 0, 0" "KeepRelativeOffset" false 1.0 1.0 0.0 0 0)
              (if (not (Variables|Default|GetbCoStarterReachLimited))
                (Variables|Default|SetbCoStarterReachLimited true)
                (Audio|SpawnSoundAttached "/Game/Project/Audio/MetaSoundSource/SE/MSS_MetalLock_4.MSS_MetalLock_4" (Variables|Default|GetSM_Mixer_Co_Starter_Handle) "None" "0, 0, 0" "0, 0, 0" "KeepRelativeOffset" false 1.0 1.0 0.0 0 0)
                (Variables|Default|SetbSoundPlaying false)
                (CallFunction|StopContinuedSE (Variables|Default|GetAudioEnable_CoStarter))))
            (else
              (CallFunction|UpdateTriggerMousePivot :!label _label_2)
              (Variables|Default|SetbCoStarterReachLimited false)
              (if (and (or (not (Utilities|IsValid (Variables|Default|GetAudioEnable_CoStarter))) (not (Variables|Default|GetbSoundPlaying))) (Variables|Default|GetbGlassCodeIsMatch))
                (Variables|Default|SetbSoundPlaying true)
                (bind _returnvalue_2 (Audio|SpawnSoundAttached "/Game/Project/Audio/MetaSoundSource/SE/MSS_ScaleSlider_6.MSS_ScaleSlider_6" (Variables|Default|GetSM_Mixer_Co_Starter_Handle) "None" "0, 0, 0" "0, 0, 0" "KeepRelativeOffset" false 1.0 1.0 0.0 0 0))
                (Variables|Default|SetAudioEnable_CoStarter _returnvalue_2))))
          (elif (>= (.z (Variables|/Script/Engine.SceneComponent|GetRelativeLocation (Variables|Default|GetSM_Mixer_Co_Starter_Handle))) (LocalVariables|GetL_LimitedLocation))
            (goto _label)
            (else
              (goto _label_2))))))))

(fn CoStarter-FinishRemainOffset
  (params (bGoingOpen :type Boolean))
  (bind _sm_mixer_co_starter_handle (Variables|Default|GetSM_Mixer_Co_Starter_Handle))
  (bind _sm_mixer_co_starter_handle_2 (Variables|Default|GetSM_Mixer_Co_Starter_Handle))
  (bind _relativelocation (Variables|/Script/Engine.SceneComponent|GetRelativeLocation _sm_mixer_co_starter_handle_2))
  (bind _relativelocation_2 (Variables|/Script/Engine.SceneComponent|GetRelativeLocation _sm_mixer_co_starter_handle))
  (bind _output_get (LocalVariables|SetL_GoingOpen bGoingOpen))
  (if _output_get
    (LocalVariables|SetL_TargetPos 144.5)
    (LocalVariables|SetL_TouchPos 145.5)
    (else
      (LocalVariables|SetL_TargetPos 194.5)
      (LocalVariables|SetL_TouchPos 193.5)))
  (Utilities|FlowControl|Sequence
    (:then_0
      (Transformation|SetRelativeLocation (Variables|Default|GetSM_Mixer_Co_Starter_Handle) (Math|Interpolation|VInterpTo (Variables|/Script/Engine.SceneComponent|GetRelativeLocation (Variables|Default|GetSM_Mixer_Co_Starter_Handle)) (Math|Vector|MakeVector (.x _relativelocation_2) (.y _relativelocation_2) (LocalVariables|GetL_TargetPos)) (Utilities|Time|GetWorldDeltaSeconds) 4.0) false false))
    (:then_1
      (if (and (LocalVariables|GetL_GoingOpen) (<= (.z (Variables|/Script/Engine.SceneComponent|GetRelativeLocation (Variables|Default|GetSM_Mixer_Co_Starter_Handle))) (LocalVariables|GetL_TouchPos)))
        (CallFunction|CheckCreateFinalItemRequest)
        (Audio|SpawnSoundAttached "/Game/Project/Audio/MetaSoundSource/SE/MSS_WoodSlide.MSS_WoodSlide" 0 "None" "0, 0, 0" "0, 0, 0" "KeepRelativeOffset" false 1.0 1.0 0.0 0 0)
        (Transformation|SetRelativeLocation _sm_mixer_co_starter_handle_2 (Math|Vector|MakeVector (.x _relativelocation) (.y _relativelocation) (LocalVariables|GetL_TargetPos)) false false :!label _label)
        (if (not (Variables|Default|GetbCoStarterReachLimited))
          (Variables|Default|SetbCoStarterReachLimited true)
          (Audio|SpawnSoundAttached "/Game/Project/Audio/MetaSoundSource/SE/MSS_MetalLock_4.MSS_MetalLock_4" (Variables|Default|GetSM_Mixer_Co_Starter_Handle) "None" "0, 0, 0" "0, 0, 0" "KeepRelativeOffset" false 1.0 1.0 0.0 0 0)
          (Variables|Default|SetbSoundPlaying false)
          (CallFunction|StopContinuedSE (Variables|Default|GetAudioEnable_CoStarter)))
        (elif (and (not (LocalVariables|GetL_GoingOpen)) (>= (.z (Variables|/Script/Engine.SceneComponent|GetRelativeLocation (Variables|Default|GetSM_Mixer_Co_Starter_Handle))) (LocalVariables|GetL_TouchPos)))
          (goto _label))))))

(fn PresetValue
  (Utilities|FlowControl|Sequence
    (:then_0
      (bind _asbp_s9007 (Utilities|Casting|CastToBP_S9007 (Variables|/Script/Engine.ChildActorComponent|GetChildActor (Variables|Default|GetFinalNotch))))
      (bind _output_get (Variables|Default|SetREF_FinalNotch _asbp_s9007))
      (Default|PlaceLocationOffset _output_get "2.108841,-5.745552,3.962831"))
    (:then_1
      (Utilities|Array|Add (Variables|S9009|GetGroupWidgetTrigger) (Variables|Default|GetWidget%20Trigger_FinalHandle))
      (Utilities|Array|Add (Variables|S9009|GetGroupWidgetTrigger) (Variables|Default|GetWidget%20Trigger_FinalItem)))
    (:then_2
      (bind _asbp_core_obj (Utilities|Casting|CastToBP_CoreOBJ (Variables|/Script/Engine.ChildActorComponent|GetChildActor (Variables|Default|GetFinalItemMesh))))
      (bind _output_get_2 (Variables|Default|SetFinalItem _asbp_core_obj))
      (Collision|SetCollisionProfileName (Variables|/Game/Project/Core/InteractOBJ/BP_CoreOBJ.BP_CoreOBJ_C|GetStaticMesh _output_get_2) "NoCollision" true :!class /Script/Engine.PrimitiveComponent)
      (Rendering|SetActorHiddenInGame (Variables|Default|GetFinalItem) true))))

(fn SwitchMeshCollisionProfile
  (params (bIsBlock :type Boolean))
  (bind _ref_finalnotch (Variables|Default|GetREF_FinalNotch))
  (bind _ref_finalnotch_2 (Variables|Default|GetREF_FinalNotch))
  (bind _setlists (Variables|/Game/Project/Core/InteractOBJ/BP_CoreOBJ_SET.BP_CoreOBJ_SET_C|GetSETLists _ref_finalnotch_2))
  (bind _setlists_2 (Variables|/Game/Project/Core/InteractOBJ/BP_CoreOBJ_SET.BP_CoreOBJ_SET_C|GetSETLists _ref_finalnotch))
  (bind _output (Utilities|Array|Get(acopy) _setlists_2))
  (bind _output_2 (Utilities|Array|Get(acopy) _setlists))
  (if bIsBlock
    (switch int (Variables|S9009|GetZoomInPart)
      (:0
        (Collision|SetCollisionProfileName (Variables|Default|GetSM_Mixer_Co_Starter_Handle) "BlockAllDynamic" true :!class /Script/Engine.PrimitiveComponent)
        (Utilities|IsValid _output
          (:Is%20Valid
            (Collision|SetCollisionProfileName (Variables|/Game/Project/Core/InteractOBJ/BP_CoreOBJ.BP_CoreOBJ_C|GetStaticMesh _output) "BlockAllDynamic" true :!class /Script/Engine.PrimitiveComponent))))
      (:1
        (if (Variables|Default|GetbFinalItemIsCreate)
          (Collision|SetCollisionProfileName (Variables|/Game/Project/Core/InteractOBJ/BP_CoreOBJ.BP_CoreOBJ_C|GetStaticMesh (Variables|Default|GetFinalItem)) "BlockAllDynamic" true :!class /Script/Engine.PrimitiveComponent))))
    (else
      (switch int (Variables|S9009|GetZoomInPart)
        (:0
          (Collision|SetCollisionProfileName (Variables|Default|GetSM_Mixer_Co_Starter_Handle) "NoCollision" true :!class /Script/Engine.PrimitiveComponent)
          (Utilities|IsValid _output_2
            (:Is%20Valid
              (Collision|SetCollisionProfileName (Variables|/Game/Project/Core/InteractOBJ/BP_CoreOBJ.BP_CoreOBJ_C|GetStaticMesh _output_2) "NoCollision" true :!class /Script/Engine.PrimitiveComponent))))
        (:1
          (Collision|SetCollisionProfileName (Variables|/Game/Project/Core/InteractOBJ/BP_CoreOBJ.BP_CoreOBJ_C|GetStaticMesh (Variables|Default|GetFinalItem)) "NoCollision" true :!class /Script/Engine.PrimitiveComponent))))))

(fn SwitchTACollisionProfile
  (params (bIsBlock :type Boolean))
  (if bIsBlock
    (for _array_element (Variables|S9009|GetGroupWidgetTrigger)
      (Collision|SetCollisionProfileName _array_element "BlockAllDynamic" true :!class /Script/Engine.PrimitiveComponent))
    (else
      (for _array_element_2 (Variables|S9009|GetGroupWidgetTrigger)
        (Collision|SetCollisionProfileName _array_element_2 "NoCollision" true :!class /Script/Engine.PrimitiveComponent)))))

(fn UpdateTriggerMousePivot
  (bind _returnvalue (Game|GetPlayerController 0))
  (Variables|S9009|SetTriggerMousePivot (.ScreenLocation (Class|PlayerController|ProjectWorldLocationtoScreen _returnvalue (.WorldLocation (Game|Player|ConvertMouseLocationToWorldSpace _returnvalue)) false))))

(fn CheckWholeMatchCode
  (Variables|Default|SetbGlassCodeIsMatch true)
  (bind _array_element (Utilities|Array|ForEachLoopwithBreak (Variables|Default|GetGlassMatchCode_QuickTest) :!label _label)
    (:LoopBody
      (if (not (Utilities|Struct|BreakST_GlassMatchCode _array_element))
        (Variables|Default|SetbGlassCodeIsMatch false)
        (goto _label Break)))))

(fn CheckSingleTotemValue
  (params (GlassValue :type ST%20Glass%20Value%20Structure))
  (LocalVariables|SetL_CurrentValue GlassValue)
  (Utilities|FlowControl|Sequence
    (:then_0
      (LocalVariables|SetL_CurrentSpline (.SplineTotem (Utilities|Struct|BreakST_GlassValue (LocalVariables|GetL_CurrentValue))))
      (LocalVariables|SetL_CurrentRotate (.Code_Rotate (Utilities|Struct|BreakST_GlassValue (LocalVariables|GetL_CurrentValue))))
      (LocalVariables|SetL_CurrentExpand (.Code_Expand (Utilities|Struct|BreakST_GlassValue (LocalVariables|GetL_CurrentValue))))
      (LocalVariables|SetL_CurrentDistance (.Code_Distance (Utilities|Struct|BreakST_GlassValue (LocalVariables|GetL_CurrentValue))))
      (LocalVariables|SetL_CurrentScale (.Code_Scale (Utilities|Struct|BreakST_GlassValue (LocalVariables|GetL_CurrentValue)))))
    (:then_1
      (bind (_array_element _array_index) (Utilities|Array|ForEachLoopwithBreak (Variables|Default|GetGlassMatchCode_QuickTest) :!label _label)
        (:LoopBody
          (bind _output_get (LocalVariables|SetL_REF_ST_GlassMatchCode _array_element))
          (LocalVariables|SetL_Index _array_index)
          (if (and (not (.bAlreadyMatch (Utilities|Struct|BreakST_GlassMatchCode _output_get))) (== (.Match_Spline (Utilities|Struct|BreakST_GlassMatchCode _output_get)) (LocalVariables|GetL_CurrentSpline)))
            (bind _bismatch (CallFunction|CheckIntDataIsInclude (LocalVariables|GetL_CurrentRotate) (.Match_Rotate (Utilities|Struct|BreakST_GlassMatchCode (LocalVariables|GetL_REF_ST_GlassMatchCode)))))
            (bind _bismatch_2 (CallFunction|CheckIntDataIsInclude (LocalVariables|GetL_CurrentExpand) (.Match_Expand (Utilities|Struct|BreakST_GlassMatchCode (LocalVariables|GetL_REF_ST_GlassMatchCode)))))
            (bind _bismatch_3 (CallFunction|CheckIntDataIsInclude (LocalVariables|GetL_CurrentDistance) (.Match_Distance (Utilities|Struct|BreakST_GlassMatchCode (LocalVariables|GetL_REF_ST_GlassMatchCode)))))
            (bind _bismatch_4 (CallFunction|CheckIntDataIsInclude (LocalVariables|GetL_CurrentScale) (.Match_Scale (Utilities|Struct|BreakST_GlassMatchCode (LocalVariables|GetL_REF_ST_GlassMatchCode)))))
            (if (Math|Boolean|ANDBoolean _bismatch_4 _bismatch_3 _bismatch_2 _bismatch)
              (bind _structout (Utilities|Struct|SetmembersinST_GlassMatchCode (LocalVariables|GetL_REF_ST_GlassMatchCode) true))
              (Utilities|Array|SetArrayElem (Variables|Default|GetGlassMatchCode_QuickTest) (LocalVariables|GetL_Index) _structout)
              (goto _label Break))))))))

(fn CheckIntDataIsInclude
  (params (CurrentValue :type Integer) (MatchCodes :type Array%20of%20Integers))
  (bind _array_element (Utilities|Array|ForEachLoopwithBreak MatchCodes :!label _label)
    (:LoopBody
      (if (== _array_element CurrentValue)
        (LocalVariables|SetL_IsMatch true)
        (goto _label Break)))
    (:Completed
      (return (LocalVariables|GetL_IsMatch)))))

(fn StartCheckMatchCode
  (for _array_element (Utilities|Struct|BreakST_GlassData (Variables|Default|GetInsertedGlass))
    (CallFunction|CheckSingleTotemValue _array_element))
  (CallFunction|CheckWholeMatchCode)
  (Development|PrintString (Utilities|String|Append "GlassCodeIsMatch = " (Utilities|String|ToString(Boolean) (Variables|Default|GetbGlassCodeIsMatch))) true true "(R=0.000000,G=0.660000,B=1.000000,A=1.000000)" 1e+01))

(fn CheckCreateFinalItemRequest
  (Utilities|FlowControl|Sequence
    (:then_0
      (Variables|Default|SetbFinalItemIsCreate true)
      (Rendering|SetActorHiddenInGame (Variables|Default|GetFinalItem) false))))

(fn FilmStateCheck
  (bind _currentsequence (Variables|Default|GetCurrentSequence))
  (if (Variables|Default|GetbPlayingFilm)
    (Utilities|IsValid _currentsequence
      (:Is%20Valid
        (Variables|Default|SetbPlayingFilm (Audio|Components|Audio|IsPlaying _currentsequence))))))