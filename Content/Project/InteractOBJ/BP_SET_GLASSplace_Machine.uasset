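; Interactable glass slot, nested as a child actor two levels inside BP_GlassCalculateMachine, that receives a glass on Interact.
; Interact unhides the glass, moves it to PlaceLocation, adds it to the parent BP_CoreOBJ_TRICK's TRICKLists and makes that trick the player's CurrentTRICK.
; UpdateGLASSCode copies the machine's updated glass code onto the inserted glass.
; Mismatch dialogue calls exist but are unconnected.
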(event EventBeginPlay
  (bind _returnvalue (Actor|GetParentActor))
  (bind _returnvalue_2 (Actor|GetParentActor _returnvalue))
  (|CallParentFunction)
  (bind _asbp_first_person_character (Utilities|Casting|CastToBP_FirstPersonCharacter (Game|GetPlayerCharacter 0)))
  (Variables|Default|SetPlayer _asbp_first_person_character)
  (Utilities|IsValid _returnvalue_2
    (:Is%20Valid
      (bind _asbp_glass_calculate_machine (Utilities|Casting|CastToBP_GlassCalculateMachine _returnvalue_2))
      (Variables|Default|SetREF_GlassCalculateMachine _asbp_glass_calculate_machine))))

(event EventInteract
  (params (InteractActor :type Actor%20Object%20Reference) (InteractTarget :type Actor%20Component%20Object%20Reference))
  (bind _asbp_glass_basetest (Utilities|Casting|CastToBP_GLASS_BASEtest InteractActor))
  (bind _output_get (Variables|Default|SetREF_InsertedGLASS _asbp_glass_basetest))
  (Development|SetHiddeninGame (Variables|/Game/Project/Core/InteractOBJ/BP_CoreOBJ.BP_CoreOBJ_C|GetStaticMesh _output_get) false false)
  (Transformation|SetActorLocation (Variables|Default|GetREF_InsertedGLASS) (Transformation|GetWorldLocation (Variables|Default|GetPlaceLocation)) false false)
  (bind _asbp_core_obj_trick (Utilities|Casting|CastToBP_CoreOBJ_TRICK (Actor|GetParentActor)))
  (Utilities|Array|Add (Variables|/Game/Project/Core/InteractOBJ/BP_CoreOBJ_TRICK.BP_CoreOBJ_TRICK_C|GetTRICKLists _asbp_core_obj_trick) (Variables|Default|GetREF_InsertedGLASS))
  (Variables|/Game/ProjectDefault/FirstPerson/Blueprints/BP_FirstPersonCharacter.BP_FirstPersonCharacter_C|SetCurrentTRICK (Variables|Default|GetPlayer) _asbp_core_obj_trick))

(fn ConstructionScript
  (|CallParentFunction))

(fn UpdateGLASSCode
  (bind _updatedglass (Default|ReturnUpdatedGLASSCode (Variables|Default|GetREF_GlassCalculateMachine)))
  (Variables|/Game/Project/InteractOBJ/BP_GLASS_BASEtest.BP_GLASS_BASEtest_C|SetThisGlass (Variables|Default|GetREF_InsertedGLASS) _updatedglass))