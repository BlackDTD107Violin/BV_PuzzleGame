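; BP_T1002 is an interactable wardrobe object that switches the player's view to a close-up of itself and back.
; Zoomin blends the camera to this actor, locks move and look input, clears the prompt UI and changes mesh collision; ZoomOut reverses the camera, input and collision.
; Both toggle ResetState on the BP_S1002 child actor from WardrobeDoor.
; InteractiveUnlocked clears IsLocked after a short delay when the received code matches.
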(event EventBeginPlay
  (|CallParentFunction)
  (bind _asbp_first_person_character (Utilities|Casting|CastToBP_FirstPersonCharacter (Game|GetPlayerCharacter 0)))
  (Variables|Default|SetPlayer _asbp_first_person_character)
  (bind _asbp_s1002 (Utilities|Casting|CastToBP_S1002 (Variables|/Script/Engine.ChildActorComponent|GetChildActor (Variables|Default|GetWardrobe_Door))))
  (Variables|Default|SetREF_%20BP%20S1002 _asbp_s1002))

(event EventInteractEnd)

(event EventZoomin
  (bind _returnvalue (Game|GetPlayerController 0))
  (Game|Player|SetViewTargetwithBlend (Game|GetPlayerController 0) self 0.5 "VTBlend_Linear" 0.0 true)
  (Input|SetIgnoreMoveInput _returnvalue true)
  (Input|SetIgnoreLookInput _returnvalue true)
  (Default|ClearGamePromptUIView (Variables|Default|GetPlayer))
  (Variables|/Game/Project/InteractOBJ/BP_S1002.BP_S1002_C|SetbResetState (Variables|Default|GetREF_%20BP%20S1002) false)
  (Collision|SetCollisionProfileName (Variables|Default|GetStaticMesh) "TRICKignore" true :!class /Script/Engine.PrimitiveComponent))

(event EventZoomOut
  (bind _returnvalue (Game|GetPlayerController 0))
  (Game|Player|SetViewTargetwithBlend (Game|GetPlayerController 0) (Game|GetPlayerCharacter 0) 0.5 "VTBlend_Linear" 0.0 true)
  (Input|ResetIgnoreMoveInput _returnvalue)
  (Input|ResetIgnoreLookInput _returnvalue)
  (Variables|/Game/Project/InteractOBJ/BP_S1002.BP_S1002_C|SetbResetState (Variables|Default|GetREF_%20BP%20S1002) true)
  (Utilities|FlowControl|Delay 0.5)
  (Collision|SetCollisionProfileName (Variables|Default|GetStaticMesh) "BlockAllDynamic" true :!class /Script/Engine.PrimitiveComponent))

(event EventInteractiveUnlocked
  (params (AttachKEY :type Actor%20Object%20Reference) (MatchOBJCode :type Name :default "None"))
  (Utilities|FlowControl|Delay 0.2)
  (if (Utilities|Enum|Equal(Enum) (Utilities|String|ToString(Name) MatchOBJCode) (Utilities|String|ToString(Name) (Variables|Default|GetSETMatchCode)))
    (Variables|Default|SetbIsLocked false)))

(fn ConstructionScript
  (|CallParentFunction))