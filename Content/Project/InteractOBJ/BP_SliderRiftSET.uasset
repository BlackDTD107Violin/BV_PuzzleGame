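; Interactable slider prop whose handle the player clicks and drags along world X, within about 50 units of its starting position.
; Each tick, when not in whole-number mode, axis input sets velocity, optionally restricted to one direction, and moves the slider.
; SetDemoMode sets axis, inertia and whole-number options and tints the slider through a dynamic material.
; Inertia sliding and whole-number snapping are unimplemented stubs, though release friction logic exists.
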(event OnBeginCursorOver(Handler)
  (params (TouchedComponent :type Primitive%20Component%20Object%20Reference))
  (Variables|Default|SetbContinueSlide true))

(event OnClicked(Handler)
  (params (TouchedComponent :type Primitive%20Component%20Object%20Reference) (ButtonPressed :type Key%20Structure :default "None"))
  (Variables|Default|SetbIsDragging true))

(event Custom|SetDemoMode
  (params (ColorType :type Integer) (bInertia :type Boolean) (bWholeNumber :type Boolean) (DirLimited :type E_AxisLimited%20Enum :default "NewEnumerator0"))
  (Variables|Default|SetColorType ColorType)
  (Variables|Default|SetbHasInertia bInertia)
  (Variables|Default|SetbWholeNumber bWholeNumber)
  (Variables|Default|SetSlideDir DirLimited)
  (bind _returnvalue (Rendering|Material|CreateDynamicMaterialInstance (Variables|Default|GetSlider) 0 "/Game/Project/MaterialLibrary/DebugOrDemo/M_TestSolidColorInstance.M_TestSolidColorInstance" "" :!class /Script/Engine.PrimitiveComponent))
  (Rendering|Material|SetVectorParameterValue _returnvalue "Tint Color" (Math|Conversions|ToLinearColor(Color) (Utilities|Array|Get(acopy) (Variables|Default|GetColorArray) (Variables|Default|GetColorType))) :!class /Script/Engine.MaterialInstanceDynamic))

(event EventBeginPlay
  (bind _returnvalue (Game|GetPlayerController 0))
  (|CallParentFunction)
  (bind _asbp_first_person_character (Utilities|Casting|CastToBP_FirstPersonCharacter (Game|GetPlayerCharacter 0)))
  (Variables|Default|SetPlayer _asbp_first_person_character)
  (Input|EnableInput _returnvalue)
  (Variables|/Script/Engine.PlayerController|SetbEnableClickEvents _returnvalue true)
  (Variables|/Script/Engine.PlayerController|SetbEnableMouseOverEvents _returnvalue true)
  (CallFunction|InitialSlideState)
  (Variables|Default|SetOrigin (Transformation|GetWorldLocation (Variables|Default|GetSlider))))

(event EventTick
  (params (DeltaSeconds :type Float%20%28single-precision%29))
  (if (Variables|Default|GetbWholeNumber)
    (if (Variables|Default|GetbIsDragging)
      _)
    (else
      (CallFunction|UpdateVelocity)
      (CallFunction|UpdateSlideMode))))

(event Input|MouseEvents|LeftMouseButton
  (params (Key :type Key%20Structure :default "None"))
  (:Released
    (Variables|Default|SetbIsDragging false)
    (Variables|Default|SetbReHandle true)
    (if (Variables|Default|GetbWholeNumber)
      _)))

(fn ConstructionScript
  (|CallParentFunction))

(fn UpdateVelocity
  (if (Variables|Default|GetbIsDragging)
    (switch Utilities|FlowControl|Switch|SwitchonE_AxisLimited (Variables|Default|GetSlideDir)
      (:NewEnumerator0
        (switch Utilities|FlowControl|Switch|SwitchonE_DirLimited (Variables|Default|GetLimitedDir)
          (:NewEnumerator0
            (Variables|Default|SetSlideVelocity (Class|Actor|GetInputAxisKeyValue) :!label _label))
          (:NewEnumerator1
            (if (> (Class|Actor|GetInputAxisKeyValue) 0.0)
              (goto _label)
              (else
                (Variables|Default|SetSlideVelocity 0.0 :!label _label_2))))
          (:NewEnumerator2
            (if (< (Class|Actor|GetInputAxisKeyValue) 0.0)
              (goto _label)
              (else
                (goto _label_2))))))
      (:NewEnumerator3
        (switch Utilities|FlowControl|Switch|SwitchonE_DirLimited (Variables|Default|GetLimitedDir)
          (:NewEnumerator0
            (Variables|Default|SetSlideVelocity (Class|Actor|GetInputAxisKeyValue) :!label _label_3))
          (:NewEnumerator1
            (if (> (Class|Actor|GetInputAxisKeyValue) 0.0)
              (goto _label_3)
              (else
                (Variables|Default|SetSlideVelocity 0.0 :!label _label_4))))
          (:NewEnumerator2
            (if (< (Class|Actor|GetInputAxisKeyValue) 0.0)
              (goto _label_3)
              (else
                (goto _label_4)))))))
    (else
      (switch Utilities|FlowControl|Switch|SwitchonE_DirLimited (Variables|Default|GetLimitedDir)
        (:NewEnumerator0
          (if (or (< (Variables|Default|GetSlideVelocity) 0.1) (> (Variables|Default|GetSlideVelocity) -0.1))
            (Variables|Default|SetSlideVelocity 0.0)
            (else
              (Variables|Default|SetSlideVelocity (* (Variables|Default|GetSlideVelocity) (Variables|Default|GetFriction))))))
        (:NewEnumerator1
          (if (< (Variables|Default|GetSlideVelocity) 0.1)
            (Variables|Default|SetSlideVelocity 0.0)
            (else
              (Variables|Default|SetSlideVelocity (* (Variables|Default|GetSlideVelocity) (Variables|Default|GetFriction))))))
        (:NewEnumerator2
          (if (> (Variables|Default|GetSlideVelocity) -0.1)
            (Variables|Default|SetSlideVelocity 0.0)
            (else
              (Variables|Default|SetSlideVelocity (* (Variables|Default|GetSlideVelocity) (Variables|Default|GetFriction))))))))))

(fn UpdateSlideMode
  (if (Variables|Default|GetbIsDragging)
    (CallFunction|SlideViaPlayerInput)
    (elif (Variables|Default|GetbHasInertia)
      (CallFunction|SlideViaInertia))))

(fn SlideViaPlayerInput
  (if (> (Variables|Default|GetSlideVelocity) 0.0)
    (if (>= (.x (Transformation|GetWorldLocation (Variables|Default|GetSlider))) (+ (.x (Variables|Default|GetOrigin)) 5e+01))
      (Development|PrintString "OutOfRange")
      (Transformation|SetWorldLocation (Variables|Default|GetSlider) (+ (Variables|Default|GetOrigin) (Math|Vector|MakeVector 5e+01 0.0 0.0)) false false)
      (else
        (Transformation|SetWorldLocation (Variables|Default|GetSlider) (+ (Transformation|GetWorldLocation (Variables|Default|GetSlider)) (Math|Vector|MakeVector (Variables|Default|GetSlideVelocity) 0.0 0.0)) false false :!label _label)))
    (elif (not (<= (.x (Transformation|GetWorldLocation (Variables|Default|GetSlider))) (+ (.x (Variables|Default|GetOrigin)) -5e+01)))
      (goto _label))))

(fn SlideViaInertia)

(fn InitialSlideState
  (Utilities|FlowControl|Sequence
    (:then_0
      (bind _output_get (Variables|Default|SetDistanceUnits (/ (.z (Transformation|GetWorldScale (Variables|Default|GetRail))) (Variables|Default|GetDividedCount))))
      (Development|PrintString (Utilities|String|ToString(Float) _output_get)))))