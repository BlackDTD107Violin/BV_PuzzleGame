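; Placement slot for the extract machine, where core objects are set down on interaction.
; On BeginPlay it caches the player character and, through a two-level parent actor lookup, the owning BP_ExtractMachine.
; Interact stores the incoming BP_CoreOBJ, unhides its mesh, moves it to PlaceLocation and adds it to the parent BP_CoreOBJ_TRICK's TRICKLists.
; Mismatch dialogue calls are unconnected, and UpdateExtractCode is empty.
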(event EventBeginPlay
  (bind _returnvalue (Actor|GetParentActor))
  (bind _returnvalue_2 (Actor|GetParentActor _returnvalue))
  (|CallParentFunction)
  (Utilities|FlowControl|Sequence
    (:then_0
      (bind _asbp_first_person_character (Utilities|Casting|CastToBP_FirstPersonCharacter (Game|GetPlayerCharacter 0)))
      (Variables|Default|SetPlayer _asbp_first_person_character))
    (:then_1
      (Utilities|IsValid _returnvalue_2
        (:Is%20Valid
          (bind _asbp_extract_machine (Utilities|Casting|CastToBP_ExtractMachine _returnvalue_2))
          (Variables|Default|SetREF_OBJExtractMachine _asbp_extract_machine))))))

(event EventInteract
  (params (InteractActor :type Actor%20Object%20Reference) (InteractTarget :type Actor%20Component%20Object%20Reference))
  (bind _asbp_core_obj (Utilities|Casting|CastToBP_CoreOBJ InteractActor))
  (bind _output_get (Variables|Default|SetREF%20Inserted%20OBJ _asbp_core_obj))
  (Development|SetHiddeninGame (Variables|/Game/Project/Core/InteractOBJ/BP_CoreOBJ.BP_CoreOBJ_C|GetStaticMesh _output_get) false false)
  (Transformation|SetActorLocation (Variables|Default|GetREF%20Inserted%20OBJ) (Transformation|GetWorldLocation (Variables|Default|GetPlaceLocation)) false false)
  (bind _asbp_core_obj_trick (Utilities|Casting|CastToBP_CoreOBJ_TRICK (Actor|GetParentActor)))
  (Utilities|Array|Add (Variables|/Game/Project/Core/InteractOBJ/BP_CoreOBJ_TRICK.BP_CoreOBJ_TRICK_C|GetTRICKLists _asbp_core_obj_trick) (Variables|Default|GetREF%20Inserted%20OBJ)))

(fn ConstructionScript
  (|CallParentFunction))

(fn UpdateExtractCode)