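; BP_O1001 is an interactable object with serial code O1001 that the first-person player can collect.
; BeginPlay sets the serial code and caches the player character as BP_FirstPersonCharacter after calling its parent.
; Its AttachtoHand function triggers the player's collection interaction, then opens dialogue entry 120101 on the player.
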(event EventBeginPlay
  (|CallParentFunction)
  (Variables|Default|SetOTHERSerialCode "O1001")
  (bind _asbp_first_person_character (Utilities|Casting|CastToBP_FirstPersonCharacter (Game|GetPlayerCharacter 0)))
  (Variables|Default|SetPlayer _asbp_first_person_character))

(fn ConstructionScript
  (|CallParentFunction))

(fn AttachtoHand
  (params (InteractTarget :type Actor%20Component%20Object%20Reference))
  (Default|InteractwithCollection (Variables|Default|GetPlayer))
  (Default|OpenDialogueTA (Variables|Default|GetPlayer) "120101")
  (return 0))