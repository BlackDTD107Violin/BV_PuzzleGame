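; BP_T0001 is a tutorial interactable that blends the player's camera onto itself for a close-up view and back out again.
; Zooming in locks move and look input and, the first time, advances the player's tutorial and clears the prompt UI.
; Zooming out restores control and advances the tutorial once more, once, if an item has been taken.
; A delayed match-code check clears its lock flag, while Interact is left empty.
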(event EventBeginPlay
  (|CallParentFunction)
  (bind _asbp_first_person_character_tutorial (Utilities|Casting|CastToBP_FirstPersonCharacterTutorial (Game|GetPlayerCharacter 0)))
  (Variables|Default|SetPlayer _asbp_first_person_character_tutorial))

(event EventZoomin
  (bind _returnvalue (Game|GetPlayerController 0))
  (bind _player (Variables|Default|GetPlayer))
  (Game|Player|SetViewTargetwithBlend (Game|GetPlayerController 0) self 0.5 "VTBlend_Linear" 0.0 true)
  (Input|SetIgnoreMoveInput _returnvalue true)
  (Input|SetIgnoreLookInput _returnvalue true)
  (if (not (Variables|Default|GetbHasTriggerTutor))
    (Variables|Default|SetbHasTriggerTutor true)
    (Utilities|FlowControl|Delay 0.5)
    (Default|ArriveTutorialTA _player)
    (Default|ClearGamePromptUIView _player)))

(event EventZoomOut
  (bind _returnvalue (Game|GetPlayerController 0))
  (Game|Player|SetViewTargetwithBlend (Game|GetPlayerController 0) (Game|GetPlayerCharacter 0) 0.5 "VTBlend_Linear" 0.0 true)
  (Input|ResetIgnoreMoveInput _returnvalue)
  (Input|ResetIgnoreLookInput _returnvalue)
  (Utilities|FlowControl|Delay 0.5)
  (if (and (not (Variables|Default|GetbItemTutorHasTrigger)) (Variables|Default|GetbHasTakeItem))
    (Variables|Default|SetbItemTutorHasTrigger true)
    (Default|ArriveTutorialTA (Variables|Default|GetPlayer))))

(event EventInteract
  (params (InteractActor :type Actor%20Object%20Reference) (InteractTarget :type Actor%20Component%20Object%20Reference)))

(event EventInteractiveUnlocked
  (params (AttachKEY :type Actor%20Object%20Reference) (MatchOBJCode :type Name :default "None"))
  (Utilities|FlowControl|Delay 0.2)
  (if (Utilities|Enum|Equal(Enum) (Utilities|String|ToString(Name) MatchOBJCode) (Utilities|String|ToString(Name) (Variables|Default|GetSETMatchCode)))
    (Variables|Default|SetbIsLocked_0 false)))

(fn ConstructionScript
  (|CallParentFunction))