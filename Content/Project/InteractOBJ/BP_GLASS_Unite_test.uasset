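; Interactable glass piece that can be picked up into an inspector and removed from a glass-placement machine slot.
; On entering inspection it plays an attach sound, hides its mesh, and frees its current trigger area by marking it empty, re-enabling collision and having the linked machine update its glass code.
; Repos hides the actor and disables collision; SetupGlass stores which glass it represents.
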(event EventBeginPlay
  (|CallParentFunction)
  (bind _asbp_core_hud (Utilities|Casting|CastToBP_CoreHUD (HUD|GetHUD (Game|GetPlayerController 0))))
  (Variables|Default|SetREF_UI_CoreHUD _asbp_core_hud))

(event EventEnterInspector
  (Audio|SpawnSoundAttached "/Game/Project/Audio/MetaSoundSource/MSS_K0001_Attach.MSS_K0001_Attach" (Variables|Default|GetStaticMesh) "None" "0, 0, 0" "0, 0, 0" "KeepRelativeOffset" false 1.0 1.0 0.0 0 0)
  (Development|SetHiddeninGame (Variables|Default|GetStaticMesh) true false)
  (Utilities|IsValid (Variables|Default|GetCurrentInsertedGLASSTA)
    (:Is%20Valid
      (Variables|/Game/Project/InteractOBJ/BP_GLASS_TA.BP_GLASS_TA_C|SetbGLASSTAIsEmpty (Variables|Default|GetCurrentInsertedGLASSTA) true)
      (Collision|SetCollisionEnabled (Variables|/Game/Project/InteractOBJ/BP_GLASS_TA.BP_GLASS_TA_C|GetKey_TriggerArea (Variables|Default|GetCurrentInsertedGLASSTA)) "QueryAndPhysics")
      (Default|UpdateGLASSCode (Variables|/Game/Project/InteractOBJ/BP_GLASS_TA.BP_GLASS_TA_C|GetREF_SET%20GLASSplace%20Machine (Variables|Default|GetCurrentInsertedGLASSTA)))
      (Variables|Default|SetCurrentInsertedGLASSTA 0))))

(event EventRepos
  (Rendering|SetActorHiddenInGame true)
  (Collision|SetActorEnableCollision false))

(fn ConstructionScript
  (|CallParentFunction))

(fn SetupGlass
  (params (Result :type ST%20Glass%20Unite%20Collection%20Structure))
  (Variables|Default|SetThisGlass Result))