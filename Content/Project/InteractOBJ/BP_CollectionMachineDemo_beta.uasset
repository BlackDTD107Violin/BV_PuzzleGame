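; Demo collection machine: an interactable puzzle prop that the player zooms into to operate.
; BeginPlay caches four child-actor controls (scale plate, slider rift, rotate and expand wheels) with their ticks off.
; Zoomin blends the view to the machine, locks player input, changes mesh collision, enables control ticks and sets wheel pivots.
; ZoomOut restores view, input and collision, stopping ticks except the expand wheel, which gets BackToDefault instead.
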(event EventBeginPlay
  (|CallParentFunction)
  (bind _asbp_first_person_character (Utilities|Casting|CastToBP_FirstPersonCharacter (Game|GetPlayerCharacter 0)))
  (Variables|Default|SetPlayer _asbp_first_person_character)
  (Utilities|FlowControl|Sequence
    (:then_0
      (bind _asbp_scale_plate_set (Utilities|Casting|CastToBP_ScalePlateSET (Variables|/Script/Engine.ChildActorComponent|GetChildActor (Variables|Default|GetScalePlate))))
      (bind _output_get (Variables|Default|SetScalePlateREF _asbp_scale_plate_set))
      (Actor|Tick|SetActorTickEnabled _output_get))
    (:then_1
      (bind _asbp_slider_rift_set_machine_demo (Utilities|Casting|CastToBP_SliderRiftSET_MachineDemo (Variables|/Script/Engine.ChildActorComponent|GetChildActor (Variables|Default|GetSliderRift))))
      (bind _output_get_2 (Variables|Default|SetSliderRiftREF _asbp_slider_rift_set_machine_demo))
      (Actor|Tick|SetActorTickEnabled _output_get_2))
    (:then_2
      (bind _asbp_rotate_wheel_set_machine_rotate (Utilities|Casting|CastToBP_RotateWheelSET_Machine_Rotate (Variables|/Script/Engine.ChildActorComponent|GetChildActor (Variables|Default|GetRotateWheel))))
      (bind _output_get_3 (Variables|Default|SetRotateWheelREF _asbp_rotate_wheel_set_machine_rotate))
      (Actor|Tick|SetActorTickEnabled _output_get_3))
    (:then_3
      (bind _asbp_rotate_wheel_set_machine_expand (Utilities|Casting|CastToBP_RotateWheelSET_Machine_Expand (Variables|/Script/Engine.ChildActorComponent|GetChildActor (Variables|Default|GetExpandWheel))))
      (bind _output_get_4 (Variables|Default|SetExpandWheelREF _asbp_rotate_wheel_set_machine_expand))
      (Actor|Tick|SetActorTickEnabled _output_get_4))))

(event EventZoomin
  (bind _returnvalue (Game|GetPlayerController 0))
  (Game|Player|SetViewTargetwithBlend (Game|GetPlayerController 0) self 0.5 "VTBlend_Linear" 0.0 true)
  (Input|SetIgnoreMoveInput _returnvalue true)
  (Input|SetIgnoreLookInput _returnvalue true)
  (Default|ClearGamePromptUIView (Variables|Default|GetPlayer))
  (Collision|SetCollisionProfileName (Variables|Default|GetStaticMesh) "TRICKignore" true :!class /Script/Engine.PrimitiveComponent)
  (Actor|Tick|SetActorTickEnabled (Variables|Default|GetScalePlateREF) true)
  (Actor|Tick|SetActorTickEnabled (Variables|Default|GetSliderRiftREF) true)
  (Actor|Tick|SetActorTickEnabled (Variables|Default|GetRotateWheelREF) true)
  (Default|SetPivotwhenZoomin (Variables|Default|GetRotateWheelREF))
  (Actor|Tick|SetActorTickEnabled (Variables|Default|GetExpandWheelREF) true)
  (Default|SetPivotwhenZoomin (Variables|Default|GetExpandWheelREF)))

(event EventZoomOut
  (bind _returnvalue (Game|GetPlayerController 0))
  (Game|Player|SetViewTargetwithBlend (Game|GetPlayerController 0) (Game|GetPlayerCharacter 0) 0.5 "VTBlend_Linear" 0.0 true)
  (Input|ResetIgnoreMoveInput _returnvalue)
  (Input|ResetIgnoreLookInput _returnvalue)
  (Collision|SetCollisionProfileName (Variables|Default|GetStaticMesh) "BlockAllDynamic" true :!class /Script/Engine.PrimitiveComponent)
  (Actor|Tick|SetActorTickEnabled (Variables|Default|GetScalePlateREF))
  (Actor|Tick|SetActorTickEnabled (Variables|Default|GetSliderRiftREF))
  (Actor|Tick|SetActorTickEnabled (Variables|Default|GetRotateWheelREF))
  (Default|BacktoDefault (Variables|Default|GetExpandWheelREF)))

(fn ConstructionScript
  (|CallParentFunction))