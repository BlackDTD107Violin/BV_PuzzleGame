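; BP_S9002 is the interactable mixer panel of the BP_S9001 machine, where the player edits a GLASS code's totem transform.
; Interacting blends the view to the panel and locks player input.
; Four child actors (Move, Turn, Mirror, Scale) receive the code's values, feed the machine's totem previewer, and are read back then reset on collection.
; A timeline drives dynamic materials to light or dim the four diamond meshes.
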(event Custom|SwitchDiamondState
  (params (bIsEnable :type Boolean))
  (if bIsEnable
    (bind (_direction _enable _speed) (Timeline|DiamondState PlayFromStart)
      (:Update
        (for _array_element (Variables|Default|GetDiamondMatGroups)
          (Rendering|Material|SetScalarParameterValue _array_element "Enable" _enable :!class /Script/Engine.MaterialInstanceDynamic)
          (Rendering|Material|SetScalarParameterValue _array_element "Speed" _speed :!class /Script/Engine.MaterialInstanceDynamic))))
    (else
      (Timeline|DiamondState ReverseFromEnd))))

(event EventBeginPlay
  (|CallParentFunction)
  (bind _asbp_first_person_character (Utilities|Casting|CastToBP_FirstPersonCharacter (Game|GetPlayerCharacter 0)))
  (Variables|Default|SetPlayer _asbp_first_person_character)
  (CallFunction|PresetValue)
  (CallFunction|PresetDiamonds))

(event EventZoomin
  (params (ZoomComponent :type Actor%20Component%20Object%20Reference))
  (bind _returnvalue (Game|GetPlayerController 0))
  (Game|Player|SetViewTargetwithBlend (Game|GetPlayerController 0) self 0.5 "VTBlend_Linear" 0.0 true)
  (Input|SetIgnoreMoveInput _returnvalue true)
  (Input|SetIgnoreLookInput _returnvalue true)
  (Default|ClearGamePromptUIView (Variables|Default|GetPlayer))
  (CallFunction|PanelActivate false))

(event EventZoomOut
  (bind _returnvalue (Game|GetPlayerController 0))
  (Game|Player|SetViewTargetwithBlend (Game|GetPlayerController 0) (Game|GetPlayerCharacter 0) 0.5 "VTBlend_Linear" 0.0 true)
  (Input|ResetIgnoreMoveInput _returnvalue)
  (Input|ResetIgnoreLookInput _returnvalue)
  (Collision|SetCollisionProfileName (Variables|Default|GetStaticMesh) "StandByMode" true :!class /Script/Engine.PrimitiveComponent))

(event EventInteract
  (params (InteractActor :type Actor%20Object%20Reference) (InteractTarget :type Actor%20Component%20Object%20Reference))
  (CallFunction|Zoomin InteractTarget))

(fn ConstructionScript
  (|CallParentFunction))

(fn AssignGLASSCodetoEachFunc
  (params (currentGLASS :type ST%20Glass%20Data%20Structure))
  (bind _output_get (Variables|Default|SetCurrentGLASS currentGLASS))
  (Default|ReceiveGLASScode (Variables|Default|GetREF_MixerTurn) (.Code_Rotate (Utilities|Struct|BreakST_GlassValue (Utilities|Array|Get(acopy) (.glassvalue _output_get)))))
  (Default|ReceiveGLASScode (Variables|Default|GetREF_MixerMirror) (- (.Code_Expand (Utilities|Struct|BreakST_GlassValue (Utilities|Array|Get(acopy) (.glassvalue _output_get)))) 1))
  (Default|ReceiveGLASScode (Variables|Default|GetREF_MixerMove) (.Code_Distance (Utilities|Struct|BreakST_GlassValue (Utilities|Array|Get(acopy) (.glassvalue _output_get)))))
  (Default|ReceiveGLASScode (Variables|Default|GetREF_MixerScale) (.Code_Scale (Utilities|Struct|BreakST_GlassValue (Utilities|Array|Get(acopy) (.glassvalue _output_get)))))
  (Default|AssignTotemPreviewer (Variables|Default|GetREF_%20MainMachine) (Variables|Default|GetCurrentGLASS) "NewEnumerator4"))

(fn ClearGLASSCode
  (Default|BacktoDefault (Variables|Default|GetREF_MixerMove))
  (Default|BacktoDefault (Variables|Default|GetREF_MixerTurn))
  (Default|BacktoDefault (Variables|Default|GetREF_MixerScale))
  (Default|BacktoDefault (Variables|Default|GetREF_MixerMirror)))

(fn CollectGLASSCodefromEachFunc
  (bind _currentglass (Variables|Default|GetCurrentGLASS))
  (bind _glassvalue (Utilities|Struct|BreakST_GlassData _currentglass))
  (bind _output (Utilities|Array|Get(acopy) _glassvalue))
  (bind (_basetotem _splinetotem) (Utilities|Struct|BreakST_GlassValue _output))
  (Utilities|Array|SetArrayElem _glassvalue 0 (Utilities|Struct|MakeST_GlassValue _basetotem _splinetotem (Variables|/Game/Project/InteractOBJ/BP_S9004.BP_S9004_C|GetInsertedGLASSUnits (Variables|Default|GetREF_MixerTurn)) (+ (Variables|/Game/Project/InteractOBJ/BP_S9005.BP_S9005_C|GetInsertedGLASSUnits (Variables|Default|GetREF_MixerMirror)) 1) (Variables|/Game/Project/InteractOBJ/BP_S9003.BP_S9003_C|GetInsertedGLASSUnits (Variables|Default|GetREF_MixerMove)) (Variables|/Game/Project/InteractOBJ/BP_S9006.BP_S9006_C|GetInsertedGLASSUnits (Variables|Default|GetREF_MixerScale))))
  (CallFunction|ClearGLASSCode)
  (return (Variables|Default|GetCurrentGLASS)))

(fn PanelActivate
  (params (bIsTurnOn :type Boolean))
  (bind _output_get (LocalVariables|SetL_IsTurnOn bIsTurnOn))
  (if _output_get
    (Collision|SetCollisionProfileName (Variables|Default|GetStaticMesh) "TRICKignore" true :!class /Script/Engine.PrimitiveComponent)
    (Actor|Tick|SetActorTickEnabled (Variables|Default|GetREF_MixerScale) (LocalVariables|GetL_IsTurnOn))
    (Actor|Tick|SetActorTickEnabled (Variables|Default|GetREF_MixerMove) (LocalVariables|GetL_IsTurnOn))
    (Actor|Tick|SetActorTickEnabled (Variables|Default|GetREF_MixerTurn) (LocalVariables|GetL_IsTurnOn))
    (Default|SetPivotwhenZoomin (Variables|Default|GetREF_MixerTurn))
    (Actor|Tick|SetActorTickEnabled (Variables|Default|GetREF_MixerMirror) (LocalVariables|GetL_IsTurnOn))
    (Default|SetPivotwhenZoomin (Variables|Default|GetREF_MixerMirror))))

(fn PresetDiamonds
  (Utilities|FlowControl|Sequence
    (:then_0
      (Utilities|Array|Add (Variables|Default|GetDiamondMeshes) (Variables|Default|GetSM_Mixer_Move_Diamond))
      (Utilities|Array|Add (Variables|Default|GetDiamondMeshes) (Variables|Default|GetSM_Mixer_Turn_Diamond))
      (Utilities|Array|Add (Variables|Default|GetDiamondMeshes) (Variables|Default|GetSM_Mixer_Mirror_Diamond))
      (Utilities|Array|Add (Variables|Default|GetDiamondMeshes) (Variables|Default|GetSM_Mixer_Scale_Diamond)))
    (:then_1
      (bind _returnvalue (Rendering|Material|CreateDynamicMaterialInstance "/Game/Project/Artist/Machine/Material/Mixer_Move_Diamond.Mixer_Move_Diamond" "None" "None" :!class /Script/Engine.KismetMaterialLibrary))
      (Utilities|Array|Add (Variables|Default|GetDiamondMatGroups) _returnvalue)
      (bind _returnvalue_2 (Rendering|Material|CreateDynamicMaterialInstance "/Game/Project/Artist/Machine/Material/Mixer_Turn_Diamond.Mixer_Turn_Diamond" "None" "None" :!class /Script/Engine.KismetMaterialLibrary))
      (Utilities|Array|Add (Variables|Default|GetDiamondMatGroups) _returnvalue_2))
    (:then_2
      (bind _returnvalue_3 (Rendering|Material|CreateDynamicMaterialInstance "/Game/Project/Artist/Machine/Material/Mixer_Mirror_Diamond.Mixer_Mirror_Diamond" "None" "None" :!class /Script/Engine.KismetMaterialLibrary))
      (Utilities|Array|Add (Variables|Default|GetDiamondMatGroups) _returnvalue_3)
      (bind _returnvalue_4 (Rendering|Material|CreateDynamicMaterialInstance "/Game/Project/Artist/Machine/Material/Mixer_Scale_Diamond.Mixer_Scale_Diamond" "None" "None" :!class /Script/Engine.KismetMaterialLibrary))
      (Utilities|Array|Add (Variables|Default|GetDiamondMatGroups) _returnvalue_4))
    (:then_3
      (for _array_element (Variables|Default|GetDiamondMatGroups)
        (Rendering|Material|SetScalarParameterValue _array_element "Enable" 0.0 :!class /Script/Engine.MaterialInstanceDynamic)
        (Rendering|Material|SetScalarParameterValue _array_element "Speed" 0.0 :!class /Script/Engine.MaterialInstanceDynamic)
        (for (_array_element_2 _array_index) (Variables|Default|GetDiamondMeshes)
          (Rendering|Material|SetMaterial _array_element_2 1 (Utilities|Array|Get(acopy) (Variables|Default|GetDiamondMatGroups) _array_index)))))))

(fn PresetValue
  (Utilities|FlowControl|Sequence
    (:then_0
      (bind _asbp_s9003 (Utilities|Casting|CastToBP_S9003 (Variables|/Script/Engine.ChildActorComponent|GetChildActor (Variables|Default|GetCA_SM_Mixer_Move))))
      (Variables|Default|SetREF_MixerMove _asbp_s9003))
    (:then_1
      (bind _asbp_s9004 (Utilities|Casting|CastToBP_S9004 (Variables|/Script/Engine.ChildActorComponent|GetChildActor (Variables|Default|GetCA_SM_Mixer_Turn))))
      (Variables|Default|SetREF_MixerTurn _asbp_s9004))
    (:then_2
      (bind _asbp_s9005 (Utilities|Casting|CastToBP_S9005 (Variables|/Script/Engine.ChildActorComponent|GetChildActor (Variables|Default|GetCA_SM_Mixer_Mirror))))
      (Variables|Default|SetREF_MixerMirror _asbp_s9005))
    (:then_3
      (bind _asbp_s9006 (Utilities|Casting|CastToBP_S9006 (Variables|/Script/Engine.ChildActorComponent|GetChildActor (Variables|Default|GetCA_SM_Mixer_Scale))))
      (Variables|Default|SetREF_MixerScale _asbp_s9006))
    (:then_4
      (bind _asbp_s9001 (Utilities|Casting|CastToBP_S9001 (Actor|GetParentActor)))
      (Variables|Default|SetREF_%20MainMachine _asbp_s9001))))

(fn ReturnInteractMesh
  (return (Variables|/Game/Project/InteractOBJ/BP_S9003.BP_S9003_C|GetSM_Mixer_Move_Handle (Variables|Default|GetREF_MixerMove)) (Variables|/Game/Project/InteractOBJ/BP_S9004.BP_S9004_C|GetSM_Mixer_Turn_Handle (Variables|Default|GetREF_MixerTurn)) (Variables|/Game/Project/InteractOBJ/BP_S9005.BP_S9005_C|GetSM_Mixer_Mirror_Handle (Variables|Default|GetREF_MixerMirror)) (Variables|/Game/Project/InteractOBJ/BP_S9006.BP_S9006_C|GetSM_Mixer_Scale_Handle (Variables|Default|GetREF_MixerScale))))

(fn UpdateGLASSCodefromEachFunc
  (Utilities|IsValid (Variables|Default|GetREF_%20MainMachine)
    (:Is%20Valid
      (Default|UpdateTotemPreviewer (Variables|Default|GetREF_%20MainMachine) (Variables|/Game/Project/InteractOBJ/BP_S9003.BP_S9003_C|GetInsertedGLASSUnits (Variables|Default|GetREF_MixerMove)) (Variables|/Game/Project/InteractOBJ/BP_S9005.BP_S9005_C|GetInsertedGLASSUnits (Variables|Default|GetREF_MixerMirror)) (Variables|/Game/Project/InteractOBJ/BP_S9004.BP_S9004_C|GetInsertedGLASSUnits (Variables|Default|GetREF_MixerTurn)) (Variables|/Game/Project/InteractOBJ/BP_S9006.BP_S9006_C|GetInsertedGLASSUnits (Variables|Default|GetREF_MixerScale))))))