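; BP_S0001 is an interactable cupboard with sliding drawers that hold child-actor objects.
; Interacting with a drawer picks open or close from its X position, plays the matching sound, and slides it with a Timeline lerp, blocking input meanwhile.
; Child objects receive the drawer through SetTempPos before the move and have IsLocked updated afterwards.
; The first completed interaction, including one on the cupboard body, advances the player's tutorial.
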(event Custom|DrawerFlipFlop
  (params (SM_REF :type Static%20Mesh%20Component%20Object%20Reference))
  (bind _relativelocation (Variables|/Script/Engine.SceneComponent|GetRelativeLocation SM_REF))
  (bind _returnvalue (>= (.x _relativelocation) 2e+01))
  (bind _returnvalue_2 (not _returnvalue))
  ;[0.05098 0.05098 0.05098] Interact
  ;;[0.05098 0.05098 0.05098] Check Drawer State then assign FlipFlop location
  (bind _output_get (Variables|Default|SetSM_REF SM_REF))
  (Variables|Default|SetStartLocation (Math|Vector|MakeVector (.x (Variables|/Script/Engine.SceneComponent|GetRelativeLocation _output_get)) (.y (Variables|/Script/Engine.SceneComponent|GetRelativeLocation _output_get)) (.z (Variables|/Script/Engine.SceneComponent|GetRelativeLocation _output_get))))
  (Variables|Default|SetEndLocation (Math|Vector|MakeVector (+ (.x (Variables|/Script/Engine.SceneComponent|GetRelativeLocation _output_get)) (Math|Float|SelectFloat 35.0 -35.0 _returnvalue_2)) (.y (Variables|/Script/Engine.SceneComponent|GetRelativeLocation _output_get)) (.z (Variables|/Script/Engine.SceneComponent|GetRelativeLocation _output_get))))
  (if _returnvalue_2
    (Audio|SpawnSoundAttached "/Game/Project/Audio/MetaSoundSource/MSS_S0001_DrawerOpen.MSS_S0001_DrawerOpen" (Variables|Default|GetSM_REF) "None" "0, 0, 0" "0, 0, 0" "KeepRelativeOffset" false 1.0 1.0 0.0 0 0)
    (else
      (Audio|SpawnSoundAttached "/Game/Project/Audio/MetaSoundSource/MSS_S0001_DrawerClose.MSS_S0001_DrawerClose" (Variables|Default|GetSM_REF) "None" "0, 0, 0" "0, 0, 0" "KeepRelativeOffset" false 1.0 1.0 0.0 0 0)))
  (for _array_element (Components|GetChildrenComponents (Variables|Default|GetSM_REF) false)
    (bind _aschild_actor_component (Utilities|Casting|CastToChildActorComponent _array_element))
    (bind _returnvalue_3 (Actor|GetActorOfClass (Variables|/Script/Engine.ChildActorComponent|GetChildActorClass _aschild_actor_component)))
    (bind _asbi_core_obj_interact_interface (Utilities|Casting|CastToBI_CoreOBJ_InteractInterface _returnvalue_3))
    (Default|SetTempPos _asbi_core_obj_interact_interface (Variables|Default|GetSM_REF))))

(event EventInteract
  (params (InteractActor :type Actor%20Object%20Reference) (InteractTarget :type Actor%20Component%20Object%20Reference))
  ;[0.05098 0.05098 0.05098] Interact
  (if (Variables|Default|GetbCanOpen)
    (Variables|Default|SetbCanOpen false)
    (bind _asstatic_mesh_component (Utilities|Casting|CastToStaticMeshComponent InteractTarget))
    (if (== _asstatic_mesh_component (Variables|Default|GetCupboard))
      (Variables|Default|SetbCanOpen true :!label _label)
      (if (Variables|Default|GetbHasTriggerTutor)
        _
        (else
          (Variables|Default|SetbHasTriggerTutor true)
          (Default|ArriveTutorialTA (Variables|Default|GetPlayer))
          (Default|ClearGamePromptUIView (Variables|Default|GetPlayer))))
      (for _array_element (Components|GetChildrenComponents (Variables|Default|GetSM_REF) false)
        (bind _aschild_actor_component (Utilities|Casting|CastToChildActorComponent _array_element))
        (bind _asbp_core_obj (Utilities|Casting|CastToBP_CoreOBJ (Variables|/Script/Engine.ChildActorComponent|GetChildActor _aschild_actor_component)))
        (Variables|/Game/Project/Core/InteractOBJ/BP_CoreOBJ.BP_CoreOBJ_C|SetbIsLocked _asbp_core_obj (Class|KismetMathLibrary|EqualExactlyVectorVector (Variables|/Script/Engine.SceneComponent|GetRelativeLocation (Variables|Default|GetSM_REF)) (Variables|Default|GetStartLocation))))
      (else
        (CallFunction|DrawerFlipFlop _asstatic_mesh_component)
        (bind _open_drawer (Timeline|Timeline PlayFromStart)
          (:Update
            (Transformation|SetRelativeLocation (Variables|Default|GetSM_REF) (Math|Vector|Lerp(Vector) (Variables|Default|GetStartLocation) (Variables|Default|GetEndLocation) _open_drawer) false false))
          (:Finished
            (goto _label)))))))

(event EventBeginPlay
  (|CallParentFunction)
  (bind _asbp_first_person_character_tutorial (Utilities|Casting|CastToBP_FirstPersonCharacterTutorial (Game|GetPlayerCharacter 0)))
  (Variables|Default|SetPlayer _asbp_first_person_character_tutorial))

(fn ConstructionScript
  (|CallParentFunction))