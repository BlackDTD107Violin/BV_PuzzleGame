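; BP_GLASS_TA is a child actor of BP_SET_GLASSplace_Machine that handles a glass inserted into that machine.
; On BeginPlay it caches the parent machine through a cast.
; RefreshInsertedGLASS stores the glass data, sends it to the machine's glass calculate machine, and calls the machine's Interact with the target glass actor.
; It then registers itself on that glass actor, unhides it and enables its collision.
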(event EventBeginPlay
  (bind _asbp_set_glassplace_machine (Utilities|Casting|CastToBP_SET_GLASSplace_Machine (Actor|GetParentActor)))
  (Variables|Default|SetREF_SET%20GLASSplace%20Machine _asbp_set_glassplace_machine))

(fn ConstructionScript)

(fn RefreshInsertedGLASS
  (params (InsertedGlass :type ST%20Glass%20Collection%20Structure))
  (Variables|Default|SetInsertedGlass InsertedGlass)
  (Default|ReceiveGLASSCode (Variables|/Game/Project/InteractOBJ/BP_SET_GLASSplace_Machine.BP_SET_GLASSplace_Machine_C|GetREF_GlassCalculateMachine (Variables|Default|GetREF_SET%20GLASSplace%20Machine)) (Variables|Default|GetInsertedGlass))
  (Default|Interact (Variables|Default|GetREF_SET%20GLASSplace%20Machine) (.TargetGlassActor (Utilities|Struct|BreakST_GlassCollection (Variables|Default|GetInsertedGlass))))
  (Variables|/Game/Project/Core/InteractOBJ/BP_CoreOBJ_GLASS.BP_CoreOBJ_GLASS_C|SetCurrentInsertedGLASSTA (.TargetGlassActor (Utilities|Struct|BreakST_GlassCollection (Variables|Default|GetInsertedGlass))) self)
  (Rendering|SetActorHiddenInGame (.TargetGlassActor (Utilities|Struct|BreakST_GlassCollection (Variables|Default|GetInsertedGlass))) false)
  (Collision|SetActorEnableCollision (.TargetGlassActor (Utilities|Struct|BreakST_GlassCollection (Variables|Default|GetInsertedGlass))) true))