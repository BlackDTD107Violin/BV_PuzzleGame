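; Trigger-area actor for insertion slots, nested in a parent actor and typed as Key, Extract or Glass.
; BeginPlay caches the parent by type, taking the notch side from Glass parents.
; Inserts reveal the item at the notch, link it back and feed its machine a code or, for most glass sides, a totem preview.
; Pick-out and reset restore emptiness and trigger collision; older mix-notch logic remains unwired.
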(event EventBeginPlay
  (switch Utilities|FlowControl|Switch|SwitchonE_TAType (Variables|Default|GetThisTAType)
    (:NewEnumerator0
      (bind _asbp_core_obj (Utilities|Casting|CastToBP_CoreOBJ (Actor|GetParentActor)))
      (Variables|Default|SetParentActor _asbp_core_obj))
    (:NewEnumerator1
      (bind _asbp_glassnotch_extract (Utilities|Casting|CastToBP_GLASSnotch_Extract (Actor|GetParentActor)))
      (Variables|Default|SetREF_OBJnotch_Extract _asbp_glassnotch_extract))
    (:NewEnumerator2
      (bind _asbp_s9007 (Utilities|Casting|CastToBP_S9007 (Actor|GetParentActor)))
      (bind _output_get (Variables|Default|SetREF%20GlassNotch _asbp_s9007))
      (Variables|Default|SetGlassTAside (Variables|/Game/Project/InteractOBJ/BP_S9007.BP_S9007_C|GetGlassNotchType _output_get))
      (Utilities|Casting|CastToBP_S9001 (Actor|GetParentActor (Variables|Default|GetREF%20GlassNotch))
        (:then
          (Variables|Default|SetbIsMainMachine true))
        (:CastFailed
          (Variables|Default|SetbIsMainMachine false))))))

(fn ConstructionScript)

(fn RefreshInsertedOBJ
  (params (InsertedOBJ :type ST%20Item%20Collection%20Structure))
  (Variables|Default|SetInsertedOBJ InsertedOBJ)
  (Default|ReceiveOBJExtractCode (Variables|/Game/Project/InteractOBJ/BP_GLASSnotch_Extract.BP_GLASSnotch_Extract_C|GetREF_OBJExtractMachine (Variables|Default|GetREF_OBJnotch_Extract)) (Variables|Default|GetInsertedOBJ))
  (Default|SpawnOBJActor (Variables|Default|GetREF_OBJnotch_Extract) (.TargetItemActor (Utilities|Struct|BreakST_ItemCollection (Variables|Default|GetInsertedOBJ))))
  (Rendering|SetActorHiddenInGame (.TargetItemActor (Utilities|Struct|BreakST_ItemCollection (Variables|Default|GetInsertedOBJ))) false)
  (Collision|SetActorEnableCollision (.TargetItemActor (Utilities|Struct|BreakST_ItemCollection (Variables|Default|GetInsertedOBJ))) true)
  (Variables|Default|SetbExtractTAIsEmpty false)
  (bind _asbp_core_obj_pickup (Utilities|Casting|CastToBP_CoreOBJ_PICKUP (.TargetItemActor (Utilities|Struct|BreakST_ItemCollection (Variables|Default|GetInsertedOBJ))))
    (:then
      (Variables|/Game/Project/Core/InteractOBJ/BP_CoreOBJ_PICKUP.BP_CoreOBJ_PICKUP_C|SetCurrentInsertedExtractTA _asbp_core_obj_pickup self))
    (:CastFailed
      (bind _asbp_core_obj_key (Utilities|Casting|CastToBP_CoreOBJ_KEY (.TargetItemActor (Utilities|Struct|BreakST_ItemCollection (Variables|Default|GetInsertedOBJ)))))
      (Variables|/Game/Project/Core/InteractOBJ/BP_CoreOBJ_KEY.BP_CoreOBJ_KEY_C|SetCurrentInsertedExtractTA _asbp_core_obj_key self))))

(fn RefreshInsertedGLASS
  (params (InsertedGlass :type ST%20Glass%20Base%20Collection%20Structure))
  (Variables|Default|SetInsertedGlass InsertedGlass)
  (if (Utilities|Enum|Equal(Enum) (Variables|Default|GetGlassTAside) "NewEnumerator4")
    (Development|PrintString "Hello")
    (Default|ReceiveGLASSCode (Variables|/Game/Project/InteractOBJ/BP_S9007.BP_S9007_C|GetREF_%20MainMachine (Variables|Default|GetREF%20GlassNotch)) (Variables|Default|GetInsertedGlass))
    (else
      (Default|AssignTotemPreviewer (Variables|/Game/Project/InteractOBJ/BP_S9007.BP_S9007_C|GetREF_%20MainMachine (Variables|Default|GetREF%20GlassNotch)) (Variables|Default|GetInsertedGlass) (Variables|Default|GetGlassTAside))))
  (Default|SpawnGlassActor (Variables|Default|GetREF%20GlassNotch) (.TargetGlassActor (Utilities|Struct|BreakST_GlassBaseCollection (Variables|Default|GetInsertedGlass))))
  (Variables|/Game/Project/Core/InteractOBJ/BP_CoreOBJ_GLASS.BP_CoreOBJ_GLASS_C|SetCurrentInsertedTA (.TargetGlassActor (Utilities|Struct|BreakST_GlassBaseCollection (Variables|Default|GetInsertedGlass))) self)
  (Rendering|SetActorHiddenInGame (.TargetGlassActor (Utilities|Struct|BreakST_GlassBaseCollection (Variables|Default|GetInsertedGlass))) false)
  (Collision|SetActorEnableCollision (.TargetGlassActor (Utilities|Struct|BreakST_GlassBaseCollection (Variables|Default|GetInsertedGlass))) true)
  (Variables|Default|SetbThisTAIsEmpty false))

(fn SetupNewGlass
  (params (Glass%20Data :type BP%20Core%20OBJ%20GLASS%20Object%20Reference))
  (LocalVariables|SetL_GlassData Glass%20Data)
  (Default|SpawnGlassActor (Variables|Default|GetREF%20GlassNotch) (LocalVariables|GetL_GlassData))
  (Variables|/Game/Project/Core/InteractOBJ/BP_CoreOBJ_GLASS.BP_CoreOBJ_GLASS_C|SetCurrentInsertedTA (LocalVariables|GetL_GlassData) self)
  (Rendering|SetActorHiddenInGame (LocalVariables|GetL_GlassData) false)
  (Collision|SetActorEnableCollision (LocalVariables|GetL_GlassData) true))

(fn ResetAfterMerge
  (Collision|SetCollisionEnabled (Variables|Default|GetKey_TriggerArea) "QueryAndPhysics")
  (Variables|Default|SetbThisTAIsEmpty true))

(fn PickOutGlass
  (Variables|Default|SetbThisTAIsEmpty true)
  (Collision|SetCollisionEnabled (Variables|Default|GetKey_TriggerArea) "QueryAndPhysics")
  (Utilities|Array|Clear (Variables|/Game/Project/Core/InteractOBJ/BP_CoreOBJ_SET.BP_CoreOBJ_SET_C|GetSETLists (Variables|Default|GetREF%20GlassNotch)))
  (return (Variables|Default|GetGlassTAside)))

(fn PickOutOBJ
  (Variables|Default|SetbExtractTAIsEmpty true)
  (Collision|SetCollisionEnabled (Variables|Default|GetKey_TriggerArea) "QueryAndPhysics")
  (Utilities|Array|Clear (Variables|/Game/Project/Core/InteractOBJ/BP_CoreOBJ_SET.BP_CoreOBJ_SET_C|GetSETLists (Variables|Default|GetREF_OBJnotch_Extract)))
  (return (Variables|Default|GetGlassTAside)))

(fn UpdateTotemandPanel
  (if (not (Variables|Default|GetbThisTAIsEmpty))
    (Default|ReceiveGLASSCode (Variables|/Game/Project/InteractOBJ/BP_S9007.BP_S9007_C|GetREF_%20MainMachine (Variables|Default|GetREF%20GlassNotch)) (Variables|Default|GetInsertedGlass))))