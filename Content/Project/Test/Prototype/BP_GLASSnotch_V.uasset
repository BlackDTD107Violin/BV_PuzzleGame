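; Glass notch slot that the player can zoom into, used inside the glass mix, extract or calculate machines.
; On BeginPlay it caches the player, its child target-area actor and whichever machine is its parent, and enables mouse click and hover events.
; Zooming blends the view to the notch and locks movement and look.
; Collision profile swaps toggle the zoom trigger, target area and placed children depending on whether the notch is occupied.
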(event EventBeginPlay
  (bind _returnvalue (Game|GetPlayerController 0))
  (bind _returnvalue_2 (Actor|GetParentActor))
  (|CallParentFunction)
  (Utilities|FlowControl|Sequence
    (:then_0
      (bind _asbp_first_person_character (Utilities|Casting|CastToBP_FirstPersonCharacter (Game|GetPlayerCharacter 0)))
      (Variables|Default|SetPlayer_0 _asbp_first_person_character)
      (Input|EnableInput _returnvalue)
      (Variables|/Script/Engine.PlayerController|SetbEnableClickEvents _returnvalue true)
      (Variables|/Script/Engine.PlayerController|SetbEnableMouseOverEvents _returnvalue true))
    (:then_1
      (bind _asbp_obj_ta (Utilities|Casting|CastToBP_OBJ_TA (Variables|/Script/Engine.ChildActorComponent|GetChildActor (Variables|Default|GetGLASS_TA))))
      (bind _output_get (Variables|Default|SetREF_OBJ%20TA _asbp_obj_ta))
      (Collision|SetCollisionProfileName (Variables|/Game/Project/BluePrints/InteractOBJ/BP_OBJ_TA.BP_OBJ_TA_C|GetKey_TriggerArea _output_get) "NoCollision" true :!class /Script/Engine.PrimitiveComponent)
      (Utilities|IsValid _returnvalue_2
        (:Is%20Valid
          (bind _asbp_glass_mix_machine (Utilities|Casting|CastToBP_GlassMixMachine _returnvalue_2)
            (:then
              (Variables|Default|SetREF_GlassMixMachine _asbp_glass_mix_machine)
              (Variables|Default|SetbIsMixMachine true))
            (:CastFailed
              (bind _asbp_extract_machine (Utilities|Casting|CastToBP_ExtractMachine (Actor|GetParentActor))
                (:then
                  (Variables|Default|SetREF_Extract%20Machine _asbp_extract_machine))
                (:CastFailed
                  (bind _asbp_glass_calculate_machine (Utilities|Casting|CastToBP_GlassCalculateMachine (Actor|GetParentActor)))
                  (Variables|Default|SetREF_GlassCalculateMachine _asbp_glass_calculate_machine))))))))))

(event EventZoomin
  (params (ZoomComponent :type Actor%20Component%20Object%20Reference))
  (bind _returnvalue (Game|GetPlayerController 0))
  (Game|Player|SetViewTargetwithBlend (Game|GetPlayerController 0) self 0.5 "VTBlend_Linear" 0.0 true)
  (Input|SetIgnoreMoveInput _returnvalue true)
  (Input|SetIgnoreLookInput _returnvalue true)
  (Default|ClearGamePromptUIView (Variables|Default|GetPlayer_0))
  (Collision|SetCollisionProfileName (Variables|Default|GetZoomTrigger_Main) "NoCollision" true :!class /Script/Engine.PrimitiveComponent)
  (if (> (Utilities|Array|Length (Variables|Default|GetChildLists)) 0)
    (Collision|SetCollisionProfileName (Variables|/Game/Project/BluePrints/InteractOBJ/BP_OBJ_TA.BP_OBJ_TA_C|GetKey_TriggerArea (Variables|Default|GetREF_OBJ%20TA)) "NoCollision" true :!class /Script/Engine.PrimitiveComponent)
    (else
      (Collision|SetCollisionProfileName (Variables|/Game/Project/BluePrints/InteractOBJ/BP_OBJ_TA.BP_OBJ_TA_C|GetKey_TriggerArea (Variables|Default|GetREF_OBJ%20TA)) "BlockAllDynamic" true :!class /Script/Engine.PrimitiveComponent))))

(event EventZoomOut
  (bind _returnvalue (Game|GetPlayerController 0))
  (Game|Player|SetViewTargetwithBlend (Game|GetPlayerController 0) (Game|GetPlayerCharacter 0) 0.5 "VTBlend_Linear" 0.0 true)
  (Input|ResetIgnoreMoveInput _returnvalue)
  (Input|ResetIgnoreLookInput _returnvalue)
  (Utilities|FlowControl|Delay 0.5)
  (Collision|SetCollisionProfileName (Variables|Default|GetZoomTrigger_Main) "BlockAllDynamic" true :!class /Script/Engine.PrimitiveComponent)
  (Collision|SetCollisionProfileName (Variables|/Game/Project/BluePrints/InteractOBJ/BP_OBJ_TA.BP_OBJ_TA_C|GetKey_TriggerArea (Variables|Default|GetREF_OBJ%20TA)) "NoCollision" true :!class /Script/Engine.PrimitiveComponent))

(fn ConstructionScript
  (|CallParentFunction))

(fn CollisionbyAutoState
  (params (bIsOpen :type Boolean))
  (if bIsOpen
    (if (> (Utilities|Array|Length (Variables|Default|GetChildLists)) 0)
      (Collision|SetCollisionProfileName (Variables|/Game/Project/BluePrints/InteractOBJ/BP_OBJ_TA.BP_OBJ_TA_C|GetKey_TriggerArea (Variables|Default|GetREF_OBJ%20TA)) "NoCollision" true :!class /Script/Engine.PrimitiveComponent)
      (for _array_element (Variables|Default|GetChildLists)
        (Collision|SetCollisionProfileName (Variables|/Game/Project/Core/InteractOBJ/BP_CoreOBJ.BP_CoreOBJ_C|GetStaticMesh _array_element) "BlockAllDynamic" true :!class /Script/Engine.PrimitiveComponent))
      (else
        (Collision|SetCollisionProfileName (Variables|/Game/Project/BluePrints/InteractOBJ/BP_OBJ_TA.BP_OBJ_TA_C|GetKey_TriggerArea (Variables|Default|GetREF_OBJ%20TA)) "BlockAllDynamic" true :!class /Script/Engine.PrimitiveComponent)))
    (else
      (Collision|SetCollisionProfileName (Variables|/Game/Project/BluePrints/InteractOBJ/BP_OBJ_TA.BP_OBJ_TA_C|GetKey_TriggerArea (Variables|Default|GetREF_OBJ%20TA)) "BlockAllDynamic" true :!class /Script/Engine.PrimitiveComponent))))