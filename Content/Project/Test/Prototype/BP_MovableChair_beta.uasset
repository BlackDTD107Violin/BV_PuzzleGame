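; Prototype chair the first-person player drags through interaction, with an optional lock cleared by a matching code.
; Interacting enables Tick and swaps collision, step-up and physics settings, then passes drag state and mass to the player.
; Tick interpolates it ahead of the player, either continuously or in distance-triggered push/pull moves that flag the player to ignore movement.
; Dragging ends outside valid range, or when the mesh hits a non-player mid-move.
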(event OnComponentHit(StaticMesh)
  (params (HitComponent :type Primitive%20Component%20Object%20Reference) (OtherActor :type Actor%20Object%20Reference) (OtherComp :type Primitive%20Component%20Object%20Reference) (NormalImpulse :type Vector :default "0, 0, 0") (Hit :type Hit%20Result%20Structure%20%28by%20ref%29))
  (Utilities|Casting|CastToBP_FirstPersonCharacter OtherActor
    (:CastFailed
      (if (Variables|Default|GetbDuringMoving)
        (Variables|Default|SetbDuringMoving false)
        (Variables|/Game/ProjectDefault/FirstPerson/Blueprints/BP_FirstPersonCharacter.BP_FirstPersonCharacter_C|SetbIgnoreMoveViaDragSET (Variables|Default|GetPlayer%20REF) false)
        (CallFunction|InteractEnd)))))

(event OnComponentHit(Chair)
  (params (HitComponent :type Primitive%20Component%20Object%20Reference) (OtherActor :type Actor%20Object%20Reference) (OtherComp :type Primitive%20Component%20Object%20Reference) (NormalImpulse :type Vector :default "0, 0, 0") (Hit :type Hit%20Result%20Structure%20%28by%20ref%29))
  (Utilities|Casting|CastToBP_FirstPersonCharacter OtherActor)
  (Default|CheckSteponSthState (Variables|Default|GetPlayer%20REF) (.z (Transformation|GetActorLocation (Game|GetPlayerCharacter 0)))))

(event EventBeginPlay
  (|CallParentFunction)
  (bind _asbp_first_person_character (Utilities|Casting|CastToBP_FirstPersonCharacter (Game|GetPlayerCharacter 0)))
  (Variables|Default|SetPlayer%20REF _asbp_first_person_character))

(event EventTick
  (params (DeltaSeconds :type Float%20%28single-precision%29))
  (CallFunction|CheckDistanceIsValid)
  (if (Variables|Default|GetbIsValidDragDistance)
    (CallFunction|UpdateDraggingState)
    (else
      (CallFunction|InteractEnd))))

(event EventInteract
  (params (InteractActor :type Actor%20Object%20Reference) (InteractTarget :type Actor%20Component%20Object%20Reference))
  (Utilities|FlowControl|Sequence
    (:then_0
      (if (or (Variables|Default|GetbInteractWithoutOBJ) (not (Variables|Default|GetbSTANDIsLocked)))
        (CallFunction|UpdateDistance)
        (Default|AssignStateDragSET (Variables|Default|GetPlayer%20REF) true (Variables|Default|GetMass))))
    (:then_1
      (if (Variables|Default|GetbSETDraggable)
        (CallFunction|OnDragSettingSwitcher true)
        (bind _output_get (Variables|Default|SetbModeSwitcher (Variables|/Game/ProjectDefault/FirstPerson/Blueprints/BP_FirstPersonCharacter.BP_FirstPersonCharacter_C|GetbDragSETmovingMode (Variables|Default|GetPlayer%20REF))))
        (if _output_get
          (Variables|Default|SetMaxValidDistance 125.0)
          (else
            (Variables|Default|SetMaxValidDistance 2e+02)))))))

(event EventInteractiveUnlocked
  (params (MatchOBJCode :type Name :default "None"))
  (if (Variables|Default|GetbSTANDIsLocked)
    (if (Utilities|Enum|Equal(Enum) (Utilities|String|ToString(Name) MatchOBJCode) (Utilities|String|ToString(Name) (Variables|Default|GetSETMatchCode)))
      (Variables|Default|SetbSTANDIsLocked false))))

(event EventInteractEnd
  (CallFunction|OnDragSettingSwitcher false))

(fn ConstructionScript
  (|CallParentFunction))

(fn UpdateDraggingState
  (if (Variables|Default|GetbModeSwitcher)
    (CallFunction|DragModeContinuous (Variables|Default|GetDistance))
    (else
      (CallFunction|DragModeMove&Stop (Variables|Default|GetDistance)))))

(fn CheckDistanceIsValid
  (bind _self self)
  (bind _player_ref (Variables|Default|GetPlayer%20REF))
  (bind _returnvalue (Transformation|GetDistanceTo _self _player_ref))
  (Variables|Default|SetbIsValidDragDistance (and (< _returnvalue (Variables|Default|GetMaxValidDistance)) (> _returnvalue (Variables|Default|GetMinValidDistance)))))

(fn SteponListUnlock
  (params (UnlockTA :type Name))
  (switch name UnlockTA
    (:K1003
      (for _array_element (Variables|Default|GetTA_K1003_StepOnList)
        (Variables|/Game/Project/Core/InteractOBJ/BP_CoreITEM.BP_CoreITEM_C|SetbCanTake _array_element false)))
    (:K1004
      (for _array_element_2 (Variables|Default|GetTA_K1004_StepOnList)
        (Variables|/Game/Project/Core/InteractOBJ/BP_CoreITEM.BP_CoreITEM_C|SetbCanTake _array_element_2 false)))))

(fn SteponListLock
  (params (UnlockTA :type Name))
  (switch name UnlockTA
    (:K1003
      (for _array_element (Variables|Default|GetTA_K1003_StepOnList)
        (Variables|/Game/Project/Core/InteractOBJ/BP_CoreITEM.BP_CoreITEM_C|SetbCanTake _array_element true)))
    (:K1004
      (for _array_element_2 (Variables|Default|GetTA_K1004_StepOnList)
        (Variables|/Game/Project/Core/InteractOBJ/BP_CoreITEM.BP_CoreITEM_C|SetbCanTake _array_element_2 true)))))

(fn DragModeContinuous
  (params (X :type Float%20%28double-precision%29))
  (bind (_outputx _outputy _outputz) (CallFunction|UpdateTargetPos X))
  (Transformation|SetActorLocation (Math|Interpolation|VInterpTo (Transformation|GetActorLocation self) (Math|Vector|MakeVector _outputx _outputy _outputz) 15.0 0.01) true false)
  (Transformation|SetWorldRotation (Variables|Default|GetStaticMesh) (Math|Rotator|MakeRotator 0.0 0.0 (+ (.yaw (Transformation|GetActorRotation (Variables|Default|GetPlayer%20REF))) 9e+01)) false false))

(fn DragModeMove&Stop
  (params (X :type Float%20%28double-precision%29))
  (bind _self self)
  (bind _player_ref (Variables|Default|GetPlayer%20REF))
  (bind _returnvalue (Transformation|GetDistanceTo _self _player_ref))
  (LocalVariables|SetLocal_XInput X)
  (if (Variables|Default|GetbDuringMoving)
    (CallFunction|SetMeshRotViaPlayerDir)
    (if (Variables|Default|GetbMove&Stop_IsPull)
      (CallFunction|SetMeshPosViaTargetPos)
      (if (<= (Transformation|GetDistanceTo self (Variables|Default|GetPlayer%20REF)) 1e+02)
        (Variables|Default|SetbDuringMoving false)
        (Variables|/Game/ProjectDefault/FirstPerson/Blueprints/BP_FirstPersonCharacter.BP_FirstPersonCharacter_C|SetbIgnoreMoveViaDragSET (Variables|Default|GetPlayer%20REF) false))
      (else
        (bind (_outputx _outputy _outputz) (CallFunction|UpdateTargetPos (+ (LocalVariables|GetLocal_XInput) 2e+01)))
        (Variables|Default|SetTempDragPos (Math|Vector|MakeVector _outputx _outputy _outputz))
        (CallFunction|SetMeshPosViaTargetPos)
        (if (>= (Transformation|GetDistanceTo self (Variables|Default|GetPlayer%20REF)) 9e+01)
          (Variables|Default|SetbDuringMoving false)
          (Variables|/Game/ProjectDefault/FirstPerson/Blueprints/BP_FirstPersonCharacter.BP_FirstPersonCharacter_C|SetbIgnoreMoveViaDragSET (Variables|Default|GetPlayer%20REF) false))))
    (else
      (bind (_outputx_2 _outputy_2 _outputz_2) (CallFunction|UpdateTargetPos (LocalVariables|GetLocal_XInput)))
      (Variables|Default|SetTempDragPos (Math|Vector|MakeVector _outputx_2 _outputy_2 _outputz_2))
      (if (>= _returnvalue 1.4e+02)
        (Variables|Default|SetbDuringMoving true)
        (Variables|Default|SetbMove&Stop_IsPull true)
        (Variables|/Game/ProjectDefault/FirstPerson/Blueprints/BP_FirstPersonCharacter.BP_FirstPersonCharacter_C|SetbIgnoreMoveViaDragSET (Variables|Default|GetPlayer%20REF) true)
        (elif (<= _returnvalue 7e+01)
          (Variables|Default|SetbDuringMoving true)
          (Variables|Default|SetbMove&Stop_IsPull false)
          (Variables|/Game/ProjectDefault/FirstPerson/Blueprints/BP_FirstPersonCharacter.BP_FirstPersonCharacter_C|SetbIgnoreMoveViaDragSET (Variables|Default|GetPlayer%20REF) true))))))

(fn SetMeshRotViaPlayerDir
  (Transformation|SetWorldRotation (Variables|Default|GetStaticMesh) (Math|Interpolation|RInterpTo (Transformation|GetWorldRotation (Variables|Default|GetStaticMesh)) (Math|Rotator|MakeRotator 0.0 0.0 (+ (.yaw (Transformation|GetActorRotation (Variables|Default|GetPlayer%20REF))) 9e+01)) 15.0 0.014) false false))

(fn UpdateTargetPos
  (params (Radius :type Float%20%28double-precision%29))
  (bind _returnvalue (Game|GetPlayerCharacter 0))
  (bind _returnvalue_2 (Math|Vector|MakeVector Radius 0.0 0.0))
  (bind _player_ref (Variables|Default|GetPlayer%20REF))
  (bind _returnvalue_3 (Transformation|GetActorRotation _player_ref))
  (bind _returnvalue_4 (Transformation|GetActorLocation _returnvalue))
  (bind _returnvalue_5 (Math|Vector|RotateVectorAroundAxis _returnvalue_2 (.yaw _returnvalue_3) "0.000000,0.000000,1.000000"))
  (return (+ (.x _returnvalue_4) (.x _returnvalue_5)) (+ (.y _returnvalue_4) (.y _returnvalue_5)) (.z _returnvalue_5)))

(fn SetMeshPosViaTargetPos
  (Transformation|SetActorLocation (Math|Interpolation|VInterpTo (Transformation|GetActorLocation self) (Variables|Default|GetTempDragPos) 15.0 0.01) true false))

(fn UpdateDistance
  (bind _output_get (Variables|Default|SetDistance (/ (Transformation|GetDistanceTo self (Variables|Default|GetPlayer%20REF)) 2.0)))
  (if (< _output_get 55.0)
    (Variables|Default|SetDistance 55.0)))

(fn OnDragSettingSwitcher
  (params (bOnInteract :type Boolean))
  (if bOnInteract
    (Actor|Tick|SetActorTickEnabled true)
    (Collision|SetCollisionProfileName (Variables|Default|GetChair) "PawnIgnore" true :!class /Script/Engine.PrimitiveComponent)
    (Physics|SetSimulatePhysics (Variables|Default|GetStaticMesh) true)
    (Collision|SetCollisionEnabled (Variables|Default|GetStaticMesh) "QueryAndPhysics")
    (Variables|/Script/Engine.PrimitiveComponent|SetCanCharacterStepUpOn (Variables|Default|GetChair) "ECB_No")
    (else
      (Actor|Tick|SetActorTickEnabled false)
      (Collision|SetCollisionProfileName (Variables|Default|GetChair) "BlockAllDynamic" true :!class /Script/Engine.PrimitiveComponent)
      (Physics|SetSimulatePhysics (Variables|Default|GetStaticMesh) false)
      (Collision|SetCollisionEnabled (Variables|Default|GetStaticMesh) "NoCollision")
      (Variables|/Script/Engine.PrimitiveComponent|SetCanCharacterStepUpOn (Variables|Default|GetChair) "ECB_Yes")
      (Default|AssignStateDragSET (Variables|Default|GetPlayer%20REF) false 0.0))))