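; Prototype glass notch, linked to its parent BP_ExtractMachine, where the player zooms in and an item can be placed.
; Zoom events blend the view, lock or restore movement and look, and toggle trigger collision, enabling the child BP_OBJ_TA key area only while the notch is empty.
; SpawnOBJActor moves an existing BP_CoreITEM to PlaceLocation, unhides and records it.
; Mismatch dialogue calls are unwired and UpdateExtractCode is empty.
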(event EventBeginPlay
  (bind _returnvalue (Actor|GetParentActor))
  (bind _returnvalue_2 (Game|GetPlayerController 0))
  (|CallParentFunction)
  (Utilities|FlowControl|Sequence
    (:then_0
      (bind _asbp_first_person_character (Utilities|Casting|CastToBP_FirstPersonCharacter (Game|GetPlayerCharacter 0)))
      (Variables|Default|SetPlayer_0 _asbp_first_person_character)
      (Input|EnableInput _returnvalue_2)
      (Variables|/Script/Engine.PlayerController|SetbEnableClickEvents _returnvalue_2 true)
      (Variables|/Script/Engine.PlayerController|SetbEnableMouseOverEvents _returnvalue_2 true))
    (:then_1
      (bind _asbp_obj_ta (Utilities|Casting|CastToBP_OBJ_TA (Variables|/Script/Engine.ChildActorComponent|GetChildActor (Variables|Default|GetGLASS_TA))))
      (bind _output_get (Variables|Default|SetREF_OBJ%20TA _asbp_obj_ta))
      (Collision|SetCollisionProfileName (Variables|/Game/Project/BluePrints/InteractOBJ/BP_OBJ_TA.BP_OBJ_TA_C|GetKey_TriggerArea _output_get) "NoCollision" true :!class /Script/Engine.PrimitiveComponent)
      (Utilities|IsValid _returnvalue
        (:Is%20Valid
          (bind _asbp_extract_machine (Utilities|Casting|CastToBP_ExtractMachine _returnvalue))
          (Variables|Default|SetREF_OBJExtractMachine _asbp_extract_machine))))))

(event EventZoomin
  (params (ZoomComponent :type Actor%20Component%20Object%20Reference))
  (bind _returnvalue (Game|GetPlayerController 0))
  (Game|Player|SetViewTargetwithBlend (Game|GetPlayerController 0) self 0.5 "VTBlend_Linear" 0.0 true)
  (Input|SetIgnoreMoveInput _returnvalue true)
  (Input|SetIgnoreLookInput _returnvalue true)
  (Default|ClearGamePromptUIView (Variables|Default|GetPlayer_0))
  (Collision|SetCollisionProfileName (Variables|Default|GetZoomTrigger_Main) "NoCollision" true :!class /Script/Engine.PrimitiveComponent)
  (if (> (Utilities|Array|Length (Variables|Default|GetChildLists)) 0)
    (Collision|SetCollisionProfileName (Variables|/Game/Project/BluePrints/InteractOBJ/BP_OBJ_TA.BP_OBJ_TA_C|GetKey_TriggerArea (Variables|Default|GetREF_OBJ%20TA)) "NoCollision" true :!class /Script/Engine.PrimitiveComponent)
    (else
      (Collision|SetCollisionProfileName (Variables|/Game/Project/BluePrints/InteractOBJ/BP_OBJ_TA.BP_OBJ_TA_C|GetKey_TriggerArea (Variables|Default|GetREF_OBJ%20TA)) "BlockAllDynamic" true :!class /Script/Engine.PrimitiveComponent))))

(event EventZoomOut
  (bind _returnvalue (Game|GetPlayerController 0))
  (Game|Player|SetViewTargetwithBlend (Game|GetPlayerController 0) (Game|GetPlayerCharacter 0) 0.5 "VTBlend_Linear" 0.0 true)
  (Input|ResetIgnoreMoveInput _returnvalue)
  (Input|ResetIgnoreLookInput _returnvalue)
  (Utilities|FlowControl|Delay 0.5)
  (Collision|SetCollisionProfileName (Variables|Default|GetZoomTrigger_Main) "BlockAllDynamic" true :!class /Script/Engine.PrimitiveComponent)
  (Collision|SetCollisionProfileName (Variables|/Game/Project/BluePrints/InteractOBJ/BP_OBJ_TA.BP_OBJ_TA_C|GetKey_TriggerArea (Variables|Default|GetREF_OBJ%20TA)) "NoCollision" true :!class /Script/Engine.PrimitiveComponent))

(fn ConstructionScript
  (|CallParentFunction))

(fn UpdateExtractCode)

(fn SpawnOBJActor
  (params (InteractTarget :type Actor%20Object%20Reference))
  (bind _asbp_core_item (Utilities|Casting|CastToBP_CoreITEM InteractTarget))
  (bind _output_get (Variables|Default|SetREF%20Inserted%20OBJ _asbp_core_item))
  (Development|SetHiddeninGame (Variables|/Game/Project/Core/InteractOBJ/BP_CoreOBJ.BP_CoreOBJ_C|GetStaticMesh _output_get) false false)
  (Transformation|SetActorLocation (Variables|Default|GetREF%20Inserted%20OBJ) (Transformation|GetWorldLocation (Variables|Default|GetPlaceLocation)) false false)
  (Utilities|Array|Add (Variables|Default|GetChildLists) (Variables|Default|GetREF%20Inserted%20OBJ)))