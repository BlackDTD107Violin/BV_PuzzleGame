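; BP_T0002 is a prototype zoomable interactable that advances the first-person tutorial.
; Zoom in blends the view to this actor, ignores player input and changes the mesh collision profile; zoom out restores them.
; One-shot flags notify the tutorial character on first zoom in and on the first zoom out after the item is taken.
; A delayed unlock event clears the locked flag when the match code fits.
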(event Custom|ZoomIn_1
  (params (ZoomComponent :type Actor%20Component%20Object%20Reference))
  (bind _returnvalue (Game|GetPlayerController 0))
  (bind _player_tutorial (Variables|Default|GetPlayer_Tutorial))
  (Utilities|FlowControl|Sequence
    (:then_0
      (Game|Player|SetViewTargetwithBlend (Game|GetPlayerController 0) self 0.5 "VTBlend_Linear" 0.0 true)
      (Input|SetIgnoreMoveInput _returnvalue true)
      (Input|SetIgnoreLookInput _returnvalue true)
      (Default|ClearGamePromptUIView (Variables|Default|GetPlayer_Tutorial))
      (Collision|SetCollisionProfileName (Variables|Default|GetStaticMesh) "TRICKignore" true :!class /Script/Engine.PrimitiveComponent))
    (:then_1
      (if (not (Variables|Default|GetbHasTriggerTutor))
        (Variables|Default|SetbHasTriggerTutor true)
        (Utilities|FlowControl|Delay 0.5)
        (Default|ArriveTutorialTA _player_tutorial)
        (Default|ClearGamePromptUIView _player_tutorial)))))

(event Custom|ZoomOut_1
  (bind _returnvalue (Game|GetPlayerController 0))
  (Utilities|FlowControl|Sequence
    (:then_0
      (Game|Player|SetViewTargetwithBlend (Game|GetPlayerController 0) (Game|GetPlayerCharacter 0) 0.5 "VTBlend_Linear" 0.0 true)
      (Input|ResetIgnoreMoveInput _returnvalue)
      (Input|ResetIgnoreLookInput _returnvalue)
      (Utilities|FlowControl|Delay 0.5)
      (Collision|SetCollisionProfileName (Variables|Default|GetStaticMesh) "BlockAllDynamic" true :!class /Script/Engine.PrimitiveComponent))
    (:then_1
      (if (and (not (Variables|Default|GetbItemTutorHasTrigger)) (Variables|Default|GetbHasTakeItem))
        (Variables|Default|SetbItemTutorHasTrigger true)
        (Default|ArriveTutorialTA (Variables|Default|GetPlayer_Tutorial))))))

(event EventBeginPlay
  (|CallParentFunction)
  (bind _asbp_first_person_character_tutorial (Utilities|Casting|CastToBP_FirstPersonCharacterTutorial (Game|GetPlayerCharacter 0)))
  (Variables|Default|SetPlayer_Tutorial _asbp_first_person_character_tutorial))

(event EventZoomOut)

(event EventInteractiveUnlocked
  (params (MatchOBJCode :type Name :default "None"))
  (Utilities|FlowControl|Delay 0.2)
  (if (Utilities|Enum|Equal(Enum) (Utilities|String|ToString(Name) MatchOBJCode) (Utilities|String|ToString(Name) (Variables|Default|GetSETMatchCode)))
    (Variables|Default|SetbSTANDIsLocked false)))

(event EventInteractEnd)

(event EventZoomin
  (params (ZoomComponent :type Actor%20Component%20Object%20Reference)))

(fn ConstructionScript
  (|CallParentFunction))