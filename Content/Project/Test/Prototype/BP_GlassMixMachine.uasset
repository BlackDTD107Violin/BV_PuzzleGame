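; Prototype mixing machine that merges the GLASS in its left and right notches into a new one in the output notch.
; Child-actor notches and slider bar are wired at BeginPlay; inserted GLASS shows on one totem previewer or fills an eight-previewer group, depending on preview type.
; A merge requires both inputs and an empty output, concatenates their values at the higher inherit layer plus one, then consumes both inputs.
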(event EventBeginPlay
  (|CallParentFunction)
  (Utilities|FlowControl|Sequence
    (:then_0
      (bind _asbp_glass_totem_previewer (Utilities|Casting|CastToBP_GlassTotemPreviewer (Variables|/Script/Engine.ChildActorComponent|GetChildActor (Variables|Default|GetGlassPreview))))
      (bind _output_get (Variables|Default|SetREF_GlassPreviewer _asbp_glass_totem_previewer))
      (Variables|/Game/Project/BluePrints/InteractOBJ/BP_GlassTotemPreviewer.BP_GlassTotemPreviewer_C|SetTotemPreviewType _output_get (Variables|Default|GetTotemPreviewType)))
    (:then_1
      (bind _asbp_mix_machine_slider_bar (Utilities|Casting|CastToBP_MixMachineSliderBar (Variables|/Script/Engine.ChildActorComponent|GetChildActor (Variables|Default|GetSliderBar))))
      (Variables|/Game/Project/Test/Prototype/BP_MixMachineSliderBar.BP_MixMachineSliderBar_C|SetREF_GlassMixMachine _asbp_mix_machine_slider_bar self))
    (:then_2
      (CallFunction|PresetEachNotch)
      (CallFunction|PresetEachPreviewerGroup))))

(fn ConstructionScript
  (|CallParentFunction))

(fn ReturnUpdatedGLASSCode)

(fn AssignTotemPreviewer
  (params (CurrentGLASS :type ST%20Glass%20Data%20Structure) (NotchSide :type E_GlassSideState%20Enum :default "NewEnumerator0"))
  (LocalVariables|SetLCurrentGlass CurrentGLASS)
  (LocalVariables|SetL_NotchSide NotchSide)
  (if (Utilities|Enum|Equal(Enum) (Variables|Default|GetTotemPreviewType) "NewEnumerator3")
    (CallFunction|AssignDatatoEachPreviewer (LocalVariables|GetLCurrentGlass) (LocalVariables|GetL_NotchSide))
    (else
      (Default|ReceiveGLASSPreviewer (Variables|Default|GetREF_GlassPreviewer) (LocalVariables|GetLCurrentGlass) (LocalVariables|GetL_NotchSide))))
  (switch Utilities|FlowControl|Switch|SwitchonE_GlassSideState (LocalVariables|GetL_NotchSide)
    (:NewEnumerator1
      (Variables|Default|SetbLeftSideIsSet true)
      (Variables|Default|SetLeftInherit (.InheritLayer (Utilities|Struct|BreakST_GlassData (LocalVariables|GetLCurrentGlass))))
      (Variables|Default|SetLeftInsertedGlass (LocalVariables|GetLCurrentGlass)))
    (:NewEnumerator2
      (Variables|Default|SetbRightSideIsSet true)
      (Variables|Default|SetRightInherit (.InheritLayer (Utilities|Struct|BreakST_GlassData (LocalVariables|GetLCurrentGlass))))
      (Variables|Default|SetRightInsertedGlass (LocalVariables|GetLCurrentGlass))))
  (if (>= (Variables|Default|GetLeftInherit) (Variables|Default|GetRightInherit))
    (Variables|Default|SetHigherInherit (Variables|Default|GetLeftInherit))
    (else
      (Variables|Default|SetHigherInherit (Variables|Default|GetRightInherit)))))

(fn EraseTotemPreviewer
  (params (Side :type E_GlassSideState%20Enum :default "NewEnumerator0"))
  (LocalVariables|SetL_NotchSide Side)
  (if (Utilities|Enum|Equal(Enum) (Variables|Default|GetTotemPreviewType) "NewEnumerator3")
    (CallFunction|RemoveDatatoEachPreviewer (LocalVariables|GetL_NotchSide))
    (else
      (Default|ClearPreviewer (Variables|Default|GetREF_GlassPreviewer) (LocalVariables|GetL_NotchSide))))
  (switch Utilities|FlowControl|Switch|SwitchonE_GlassSideState (LocalVariables|GetL_NotchSide)
    (:NewEnumerator1
      (Variables|Default|SetbLeftSideIsSet false)
      (Variables|Default|SetLeftInherit -999)
      (Variables|Default|SetHigherInherit (Variables|Default|GetRightInherit))
      (Variables|Default|SetLeftInsertedGlass ""))
    (:NewEnumerator2
      (Variables|Default|SetbRightSideIsSet false)
      (Variables|Default|SetRightInherit -999)
      (Variables|Default|SetHigherInherit (Variables|Default|GetLeftInherit))
      (Variables|Default|SetRightInsertedGlass ""))))

(fn CheckMergeRequest
  (if (Math|Boolean|ANDBoolean (Variables|Default|GetbLeftSideIsSet) (Variables|Default|GetbRightSideIsSet) (Variables|Default|GetbMixNotchIsEmpty))
    (for _array_element (.glassvalue (Variables|Default|GetLeftInsertedGlass))
      (Utilities|Array|Add (LocalVariables|GetL_MixInsertedGlass) _array_element))
    (for _array_element_2 (.glassvalue (Variables|Default|GetRightInsertedGlass))
      (Utilities|Array|Add (LocalVariables|GetL_MixInsertedGlass) _array_element_2))
    (bind _asbp_glassnotch_mix (Utilities|Casting|CastToBP_GLASSnotch_Mix (Variables|/Script/Engine.ChildActorComponent|GetChildActor (Variables|Default|GetGLASSNotch_Mix))))
    (Default|ReceiveMixDataandCreate _asbp_glassnotch_mix (Utilities|Struct|MakeST_GlassData 0 -1 (+ (Variables|Default|GetHigherInherit) 1) (LocalVariables|GetL_MixInsertedGlass) 0 0 0))
    (CallFunction|ConsumeMergeGlassandReset)
    (elif (Variables|Default|GetbMixNotchIsEmpty)
      (Development|PrintString "Side Notch Is Empty")
      (else
        (Development|PrintString "Mix Notch Has Glass")))))

(fn PresetEachNotch
  (Utilities|FlowControl|Sequence
    (:then_0
      (bind _asbp_glassnotch_mix (Utilities|Casting|CastToBP_GLASSnotch_Mix (Variables|/Script/Engine.ChildActorComponent|GetChildActor (Variables|Default|GetGLASSNotch_Left))))
      (Default|SetupGlassTAside _asbp_glassnotch_mix "NewEnumerator1"))
    (:then_1
      (bind _asbp_glassnotch_mix_2 (Utilities|Casting|CastToBP_GLASSnotch_Mix (Variables|/Script/Engine.ChildActorComponent|GetChildActor (Variables|Default|GetGLASSNotch_Right))))
      (Default|SetupGlassTAside _asbp_glassnotch_mix_2 "NewEnumerator2"))
    (:then_2
      (bind _asbp_glassnotch_mix_3 (Utilities|Casting|CastToBP_GLASSnotch_Mix (Variables|/Script/Engine.ChildActorComponent|GetChildActor (Variables|Default|GetGLASSNotch_Mix))))
      (Default|SetupGlassTAside _asbp_glassnotch_mix_3 "NewEnumerator3")
      (Variables|/Game/Project/Test/Prototype/BP_GLASSnotch_Mix.BP_GLASSnotch_Mix_C|SetREF_GlassPool _asbp_glassnotch_mix_3 (Variables|Default|GetREF_GlassPool)))))

(fn ConsumeMergeGlassandReset
  (Utilities|FlowControl|Sequence
    (:then_0
      (Variables|Default|SetbMixNotchIsEmpty false)
      (Variables|Default|SetbLeftSideIsSet false)
      (Variables|Default|SetbRightSideIsSet false)
      (Variables|Default|SetLeftInsertedGlass "")
      (Variables|Default|SetRightInsertedGlass ""))
    (:then_1
      (bind _asbp_glassnotch_mix (Utilities|Casting|CastToBP_GLASSnotch_Mix (Variables|/Script/Engine.ChildActorComponent|GetChildActor (Variables|Default|GetGLASSNotch_Left))))
      (Default|CallConsumeThisGlass (Variables|/Game/Project/Test/Prototype/BP_GLASSnotch_Mix.BP_GLASSnotch_Mix_C|GetREF_InsertedGLASS _asbp_glassnotch_mix) (Variables|/Game/Project/Test/Prototype/BP_GLASSnotch_Mix.BP_GLASSnotch_Mix_C|GetREF_InsertedGLASS _asbp_glassnotch_mix))
      (bind _asbp_obj_ta (Utilities|Casting|CastToBP_OBJ_TA (Variables|/Script/Engine.ChildActorComponent|GetChildActor (Variables|/Game/Project/Test/Prototype/BP_GLASSnotch_Mix.BP_GLASSnotch_Mix_C|GetGLASS_TA _asbp_glassnotch_mix))))
      (Default|ResetAfterMerge _asbp_obj_ta)
      (Default|RemoveGlassTAside _asbp_glassnotch_mix "NewEnumerator1"))
    (:then_2
      (bind _asbp_glassnotch_mix_2 (Utilities|Casting|CastToBP_GLASSnotch_Mix (Variables|/Script/Engine.ChildActorComponent|GetChildActor (Variables|Default|GetGLASSNotch_Right))))
      (Default|CallConsumeThisGlass (Variables|/Game/Project/Test/Prototype/BP_GLASSnotch_Mix.BP_GLASSnotch_Mix_C|GetREF_InsertedGLASS _asbp_glassnotch_mix_2) (Variables|/Game/Project/Test/Prototype/BP_GLASSnotch_Mix.BP_GLASSnotch_Mix_C|GetREF_InsertedGLASS _asbp_glassnotch_mix_2))
      (bind _asbp_obj_ta_2 (Utilities|Casting|CastToBP_OBJ_TA (Variables|/Script/Engine.ChildActorComponent|GetChildActor (Variables|/Game/Project/Test/Prototype/BP_GLASSnotch_Mix.BP_GLASSnotch_Mix_C|GetGLASS_TA _asbp_glassnotch_mix_2))))
      (Default|ResetAfterMerge _asbp_obj_ta_2)
      (Default|RemoveGlassTAside _asbp_glassnotch_mix_2 "NewEnumerator2"))))

(fn PresetEachPreviewerGroup
  (Utilities|FlowControl|Sequence
    (:then_0
      (bind _asbp_glass_totem_previewer (Utilities|Casting|CastToBP_GlassTotemPreviewer (Variables|/Script/Engine.ChildActorComponent|GetChildActor (Variables|Default|GetGlassPreview))))
      (Utilities|Array|Add (Variables|Default|GetPreviewGroup) _asbp_glass_totem_previewer)
      (bind _asbp_glass_totem_previewer_2 (Utilities|Casting|CastToBP_GlassTotemPreviewer (Variables|/Script/Engine.ChildActorComponent|GetChildActor (Variables|Default|GetGlassPreview1))))
      (Utilities|Array|Add (Variables|Default|GetPreviewGroup) _asbp_glass_totem_previewer_2))
    (:then_1
      (bind _asbp_glass_totem_previewer_3 (Utilities|Casting|CastToBP_GlassTotemPreviewer (Variables|/Script/Engine.ChildActorComponent|GetChildActor (Variables|Default|GetGlassPreview2))))
      (Utilities|Array|Add (Variables|Default|GetPreviewGroup) _asbp_glass_totem_previewer_3)
      (bind _asbp_glass_totem_previewer_4 (Utilities|Casting|CastToBP_GlassTotemPreviewer (Variables|/Script/Engine.ChildActorComponent|GetChildActor (Variables|Default|GetGlassPreview3))))
      (Utilities|Array|Add (Variables|Default|GetPreviewGroup) _asbp_glass_totem_previewer_4))
    (:then_2
      (bind _asbp_glass_totem_previewer_5 (Utilities|Casting|CastToBP_GlassTotemPreviewer (Variables|/Script/Engine.ChildActorComponent|GetChildActor (Variables|Default|GetGlassPreview4))))
      (Utilities|Array|Add (Variables|Default|GetPreviewGroup) _asbp_glass_totem_previewer_5)
      (bind _asbp_glass_totem_previewer_6 (Utilities|Casting|CastToBP_GlassTotemPreviewer (Variables|/Script/Engine.ChildActorComponent|GetChildActor (Variables|Default|GetGlassPreview5))))
      (Utilities|Array|Add (Variables|Default|GetPreviewGroup) _asbp_glass_totem_previewer_6))
    (:then_3
      (bind _asbp_glass_totem_previewer_7 (Utilities|Casting|CastToBP_GlassTotemPreviewer (Variables|/Script/Engine.ChildActorComponent|GetChildActor (Variables|Default|GetGlassPreview6))))
      (Utilities|Array|Add (Variables|Default|GetPreviewGroup) _asbp_glass_totem_previewer_7)
      (bind _asbp_glass_totem_previewer_8 (Utilities|Casting|CastToBP_GlassTotemPreviewer (Variables|/Script/Engine.ChildActorComponent|GetChildActor (Variables|Default|GetGlassPreview7))))
      (Utilities|Array|Add (Variables|Default|GetPreviewGroup) _asbp_glass_totem_previewer_8))
    (:then_4
      (for _array_element (Variables|Default|GetPreviewGroup)
        (Variables|/Game/Project/BluePrints/InteractOBJ/BP_GlassTotemPreviewer.BP_GlassTotemPreviewer_C|SetTotemPreviewType _array_element (Variables|Default|GetTotemPreviewType))))))

(fn AssignDatatoEachPreviewer
  (params (LCurrentGlass :type ST%20Glass%20Data%20Structure) (ValueSide :type E_GlassSideState%20Enum :default "NewEnumerator0"))
  (bind _output_get (LocalVariables|SetL_CurrentGlass LCurrentGlass))
  (LocalVariables|SetL_GlassValueCount_Total (Utilities|Array|Length (.GlassValue (Utilities|Struct|BreakST_GlassData _output_get))))
  (LocalVariables|SetL_NotchSide ValueSide)
  (bind _index (Utilities|FlowControl|ForLoopwithBreak 0 7 :!label _label)
    (:LoopBody
      (if (Utilities|Enum|Equal(Enum) (Variables|/Game/Project/BluePrints/InteractOBJ/BP_GlassTotemPreviewer.BP_GlassTotemPreviewer_C|GetCurrentActivateSide (Utilities|Array|Get(acopy) (Variables|Default|GetPreviewGroup) _index)) "NewEnumerator0")
        (Default|ReceiveGLASSPreviewer :self (Utilities|Array|Get(acopy) (Variables|Default|GetPreviewGroup) _index) :ValueSide (LocalVariables|GetL_NotchSide) :CurrentGlassValue (Utilities|Array|Get(acopy) (.GlassValue (Utilities|Struct|BreakST_GlassData LCurrentGlass)) (LocalVariables|GetL_GlassValueCount)))
        (bind _output_get_2 (LocalVariables|SetL_GlassValueCount (+ (LocalVariables|GetL_GlassValueCount) 1)))
        (if (== _output_get_2 (LocalVariables|GetL_GlassValueCount_Total))
          (goto _label Break))))))

(fn RemoveDatatoEachPreviewer
  (params (Side :type E_GlassSideState%20Enum :default "NewEnumerator0"))
  (LocalVariables|SetL_NotchSide Side)
  (for _index (range 0 7)
    (if (Utilities|Enum|Equal(Enum) (Variables|/Game/Project/BluePrints/InteractOBJ/BP_GlassTotemPreviewer.BP_GlassTotemPreviewer_C|GetCurrentActivateSide (Utilities|Array|Get(acopy) (Variables|Default|GetPreviewGroup) _index)) (LocalVariables|GetL_NotchSide))
      (Default|ClearPreviewer (Utilities|Array|Get(acopy) (Variables|Default|GetPreviewGroup) _index) (LocalVariables|GetL_NotchSide)))))