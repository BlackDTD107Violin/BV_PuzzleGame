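; Prototype control station, parented to BP_GlassCalculateMachine, where the player zooms in to edit a GLASS code through four child-actor controls: scale plate, distance slider, rotate and expand wheels.
; Zoom in blends the view to the station, locks player input and enables the controls' ticks, which start disabled.
; It distributes codes to the controls, updates the machine's totem previewer and collects edited values, offsetting Expand by one, then resets.
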(event EventBeginPlay
  (|CallParentFunction)
  (bind _asbp_first_person_character (Utilities|Casting|CastToBP_FirstPersonCharacter (Game|GetPlayerCharacter 0)))
  (Variables|Default|SetPlayer_0 _asbp_first_person_character)
  (bind _asbp_glass_calculate_machine (Utilities|Casting|CastToBP_GlassCalculateMachine (Actor|GetParentActor)))
  (Variables|Default|SetREF_Glass%20Calculate%20Machine _asbp_glass_calculate_machine)
  (Utilities|FlowControl|Sequence
    (:then_0
      (bind _asbp_scale_plate_set_machine_scale (Utilities|Casting|CastToBP_ScalePlateSET_Machine_Scale (Variables|/Script/Engine.ChildActorComponent|GetChildActor (Variables|Default|GetPlate_Scale))))
      (bind _output_get (Variables|Default|SetScalePlateREF _asbp_scale_plate_set_machine_scale))
      (Actor|Tick|SetActorTickEnabled _output_get))
    (:then_1
      (bind _asbp_slider_rift_set_machine_distance (Utilities|Casting|CastToBP_SliderRiftSET_Machine_Distance (Variables|/Script/Engine.ChildActorComponent|GetChildActor (Variables|Default|GetSlider_Distance))))
      (bind _output_get_2 (Variables|Default|SetSliderRiftREF _asbp_slider_rift_set_machine_distance))
      (Actor|Tick|SetActorTickEnabled _output_get_2))
    (:then_2
      (bind _asbp_rotate_wheel_set_machine_rotate (Utilities|Casting|CastToBP_RotateWheelSET_Machine_Rotate (Variables|/Script/Engine.ChildActorComponent|GetChildActor (Variables|Default|GetWheel_Rotate))))
      (bind _output_get_3 (Variables|Default|SetRotateWheelREF _asbp_rotate_wheel_set_machine_rotate))
      (Actor|Tick|SetActorTickEnabled _output_get_3))
    (:then_3
      (bind _asbp_rotate_wheel_set_machine_expand (Utilities|Casting|CastToBP_RotateWheelSET_Machine_Expand (Variables|/Script/Engine.ChildActorComponent|GetChildActor (Variables|Default|GetWheel_Expand))))
      (bind _output_get_4 (Variables|Default|SetExpandWheelREF _asbp_rotate_wheel_set_machine_expand))
      (Actor|Tick|SetActorTickEnabled _output_get_4))))

(event EventZoomin
  (params (ZoomComponent :type Actor%20Component%20Object%20Reference))
  (bind _returnvalue (Game|GetPlayerController 0))
  (Game|Player|SetViewTargetwithBlend (Game|GetPlayerController 0) self 0.5 "VTBlend_Linear" 0.0 true)
  (Input|SetIgnoreMoveInput _returnvalue true)
  (Input|SetIgnoreLookInput _returnvalue true)
  (Default|ClearGamePromptUIView (Variables|Default|GetPlayer_0))
  (Collision|SetCollisionProfileName (Variables|Default|GetStaticMesh) "TRICKignore" true :!class /Script/Engine.PrimitiveComponent)
  (Actor|Tick|SetActorTickEnabled (Variables|Default|GetScalePlateREF) true)
  (Actor|Tick|SetActorTickEnabled (Variables|Default|GetSliderRiftREF) true)
  (Actor|Tick|SetActorTickEnabled (Variables|Default|GetRotateWheelREF) true)
  (Default|SetPivotwhenZoomin (Variables|Default|GetRotateWheelREF))
  (Actor|Tick|SetActorTickEnabled (Variables|Default|GetExpandWheelREF) true)
  (Default|SetPivotwhenZoomin (Variables|Default|GetExpandWheelREF)))

(event EventZoomOut
  (bind _returnvalue (Game|GetPlayerController 0))
  (Game|Player|SetViewTargetwithBlend (Game|GetPlayerController 0) (Game|GetPlayerCharacter 0) 0.5 "VTBlend_Linear" 0.0 true)
  (Input|ResetIgnoreMoveInput _returnvalue)
  (Input|ResetIgnoreLookInput _returnvalue)
  (Collision|SetCollisionProfileName (Variables|Default|GetStaticMesh) "BlockAllDynamic" true :!class /Script/Engine.PrimitiveComponent))

(fn ConstructionScript
  (|CallParentFunction))

(fn AssignGLASSCodetoEachFunc
  (params (CurrentGLASS :type ST%20Glass%20Data%20Structure))
  (bind _output_get (Variables|Default|SetCurrentGLASS CurrentGLASS))
  (Default|ReceiveGLASScode (Variables|Default|GetRotateWheelREF) (.Code_Rotate (Utilities|Struct|BreakST_GlassValue (Utilities|Array|Get(acopy) (.glassvalue _output_get)))))
  (Default|ReceiveGLASScode (Variables|Default|GetExpandWheelREF) (- (.Code_Expand (Utilities|Struct|BreakST_GlassValue (Utilities|Array|Get(acopy) (.glassvalue _output_get)))) 1))
  (Default|ReceiveGLASScode (Variables|Default|GetSliderRiftREF) (.Code_Distance (Utilities|Struct|BreakST_GlassValue (Utilities|Array|Get(acopy) (.glassvalue _output_get)))))
  (Default|ReceiveGLASScode (Variables|Default|GetScalePlateREF) (.Code_Scale (Utilities|Struct|BreakST_GlassValue (Utilities|Array|Get(acopy) (.glassvalue _output_get)))))
  (Default|AssignTotemPreviewer (Variables|Default|GetREF_Glass%20Calculate%20Machine) (Variables|Default|GetCurrentGLASS)))

(fn CollectGLASSCodefromEachFunc
  (bind _currentglass (Variables|Default|GetCurrentGLASS))
  (bind _glassvalue (Utilities|Struct|BreakST_GlassData _currentglass))
  (bind _output (Utilities|Array|Get(acopy) _glassvalue))
  (bind (_basetotem _splinetotem) (Utilities|Struct|BreakST_GlassValue _output))
  (Utilities|Array|SetArrayElem _glassvalue 0 (Utilities|Struct|MakeST_GlassValue _basetotem _splinetotem (Variables|/Game/Project/Test/Prototype/BP_RotateWheelSET_Machine_Rotate.BP_RotateWheelSET_Machine_Rotate_C|GetInsertedGLASSUnits (Variables|Default|GetRotateWheelREF)) (+ (Variables|/Game/Project/Test/Prototype/BP_RotateWheelSET_Machine_Expand.BP_RotateWheelSET_Machine_Expand_C|GetInsertedGLASSUnits (Variables|Default|GetExpandWheelREF)) 1) (Variables|/Game/Project/Test/Prototype/BP_SliderRiftSET_Machine_Distance.BP_SliderRiftSET_Machine_Distance_C|GetInsertedGLASSUnits (Variables|Default|GetSliderRiftREF)) (Variables|/Game/Project/Test/Prototype/BP_ScalePlateSET_Machine_Scale.BP_ScalePlateSET_Machine_Scale_C|GetInsertedGLASSUnits (Variables|Default|GetScalePlateREF))))
  (CallFunction|ClearGLASSCode)
  (return (Variables|Default|GetCurrentGLASS)))

(fn ClearGLASSCode
  (Default|BacktoDefault (Variables|Default|GetScalePlateREF))
  (Default|BacktoDefault (Variables|Default|GetSliderRiftREF))
  (Default|BacktoDefault (Variables|Default|GetRotateWheelREF))
  (Default|BacktoDefault (Variables|Default|GetExpandWheelREF)))

(fn UpdateGLASSCodefromEachFunc
  (Utilities|IsValid (Variables|Default|GetREF_Glass%20Calculate%20Machine)
    (:Is%20Valid
      (Default|UpdateTotemPreviewer (Variables|Default|GetREF_Glass%20Calculate%20Machine) (Variables|/Game/Project/Test/Prototype/BP_SliderRiftSET_Machine_Distance.BP_SliderRiftSET_Machine_Distance_C|GetInsertedGLASSUnits (Variables|Default|GetSliderRiftREF)) (Variables|/Game/Project/Test/Prototype/BP_RotateWheelSET_Machine_Expand.BP_RotateWheelSET_Machine_Expand_C|GetInsertedGLASSUnits (Variables|Default|GetExpandWheelREF)) (Variables|/Game/Project/Test/Prototype/BP_RotateWheelSET_Machine_Rotate.BP_RotateWheelSET_Machine_Rotate_C|GetInsertedGLASSUnits (Variables|Default|GetRotateWheelREF)) (Variables|/Game/Project/Test/Prototype/BP_ScalePlateSET_Machine_Scale.BP_ScalePlateSET_Machine_Scale_C|GetInsertedGLASSUnits (Variables|Default|GetScalePlateREF))))))