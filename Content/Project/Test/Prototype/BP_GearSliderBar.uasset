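; Interactive gear slider bar with a zoom-in view that the player pulls by mouse drag to open the drawer on a referenced calculate machine.
; Tick turns downward mouse movement into pivot roll and scrubs the gear's start time offset to match.
; On release, the bar eases to completion if pulled far enough, otherwise springs back.
; Zooming out auto-closes the drawer and lets the locked bar return to rest.
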(event OnClicked(SlideBar)
  (params (TouchedComponent :type Primitive%20Component%20Object%20Reference) (ButtonPressed :type Key%20Structure))
  (if (Variables|Default|GetbSlideBarIsFinish)
    (Variables|Default|SetbIsDraggingSlider false)
    (else
      (Variables|Default|SetbIsDraggingSlider true)
      (Variables|/Game/ProjectDefault/FirstPerson/Blueprints/BP_FirstPersonCharacter.BP_FirstPersonCharacter_C|SetCurrentInteract (Variables|Default|GetPlayer_0) self))))

(event EventBeginPlay
  (bind _returnvalue (Game|GetPlayerController 0))
  (|CallParentFunction)
  (bind _asbp_first_person_character (Utilities|Casting|CastToBP_FirstPersonCharacter (Game|GetPlayerCharacter 0)))
  (Variables|Default|SetPlayer_0 _asbp_first_person_character)
  (Input|EnableInput _returnvalue)
  (Variables|/Script/Engine.PlayerController|SetbEnableClickEvents _returnvalue true)
  (Variables|/Script/Engine.PlayerController|SetbEnableMouseOverEvents _returnvalue true))

(event EventTick
  (params (DeltaSeconds :type Float%20%28single-precision%29))
  (if (not (Variables|Default|GetbSlideBarIsFinish))
    (CallFunction|CheckSliderState)))

(event EventInteractEnd
  (CallFunction|CancelingDrag)
  (Variables|/Game/ProjectDefault/FirstPerson/Blueprints/BP_FirstPersonCharacter.BP_FirstPersonCharacter_C|SetCurrentInteract (Variables|Default|GetPlayer_0) self)
  (Variables|Default|SetbSoundPlaying false))

(event EventZoomin
  (params (ZoomComponent :type Actor%20Component%20Object%20Reference))
  (bind _returnvalue (Game|GetPlayerController 0))
  (Game|Player|SetViewTargetwithBlend (Game|GetPlayerController 0) self 0.5 "VTBlend_Linear" 0.0 true)
  (Input|SetIgnoreMoveInput _returnvalue true)
  (Input|SetIgnoreLookInput _returnvalue true)
  (Default|ClearGamePromptUIView (Variables|Default|GetPlayer_0))
  (Collision|SetCollisionProfileName (Variables|Default|GetZoomTrigger_Main) "NoCollision" true :!class /Script/Engine.PrimitiveComponent))

(event EventZoomOut
  (bind _returnvalue (Game|GetPlayerController 0))
  (bind _ref_calculatemachine (Variables|Default|GetREF_CalculateMachine))
  (Game|Player|SetViewTargetwithBlend (Game|GetPlayerController 0) (Game|GetPlayerCharacter 0) 0.5 "VTBlend_Linear" 0.0 true)
  (Input|ResetIgnoreMoveInput _returnvalue)
  (Input|ResetIgnoreLookInput _returnvalue)
  (Variables|/Game/Project/Test/Prototype/BP_GlassCalculateMachine_V.BP_GlassCalculateMachine_V_C|SetbDrawerIsAuto _ref_calculatemachine true)
  (Variables|/Game/Project/Test/Prototype/BP_GlassCalculateMachine_V.BP_GlassCalculateMachine_V_C|SetbIsAutoOpen _ref_calculatemachine false)
  (Utilities|FlowControl|Delay 0.5)
  (Variables|Default|SetbIsDraggingSlider false)
  (Variables|Default|SetbSlideBarIsFinish false)
  (Utilities|FlowControl|Delay 0.5)
  (Collision|SetCollisionProfileName (Variables|Default|GetZoomTrigger_Main) "BlockAllDynamic" true :!class /Script/Engine.PrimitiveComponent))

(fn ConstructionScript
  (|CallParentFunction))

(fn UpdateTriggerMousePivot
  (bind _returnvalue (Game|GetPlayerController 0))
  (Variables|Default|SetTriggerMousePivot (.ScreenLocation (Class|PlayerController|ProjectWorldLocationtoScreen _returnvalue (.WorldLocation (Game|Player|ConvertMouseLocationToWorldSpace _returnvalue)) false))))

(fn CancelingDrag
  (Variables|Default|SetbIsDraggingSlider false)
  (Variables|Default|SetbHasUpdateMousePivot false))

(fn FinishRemainingAngleCover
  (bind _slidebarpivot (Variables|Default|GetSlideBarPivot))
  (bind _slidebarpivot_2 (Variables|Default|GetSlideBarPivot))
  (bind _ref_calculatemachine (Variables|Default|GetREF_CalculateMachine))
  (bind _relativerotation (Variables|/Script/Engine.SceneComponent|GetRelativeRotation _slidebarpivot))
  (bind _relativerotation_2 (Variables|/Script/Engine.SceneComponent|GetRelativeRotation _slidebarpivot_2))
  (Utilities|FlowControl|Sequence
    (:then_0
      (Transformation|SetRelativeRotation (Variables|Default|GetSlideBarPivot) (Math|Interpolation|RInterpTo (Variables|/Script/Engine.SceneComponent|GetRelativeRotation (Variables|Default|GetSlideBarPivot)) (Math|Rotator|MakeRotator -75.0 (.pitch _relativerotation) (.yaw _relativerotation)) (Utilities|Time|GetWorldDeltaSeconds) 4.0) false false))
    (:then_1
      (if (<= (.roll (Variables|/Script/Engine.SceneComponent|GetRelativeRotation (Variables|Default|GetSlideBarPivot))) -74.0)
        (Transformation|SetRelativeRotation (Variables|Default|GetSlideBarPivot) (Math|Rotator|MakeRotator -75.0 (.pitch _relativerotation_2) (.yaw _relativerotation_2)) false false)
        (Variables|Default|SetbSlideBarIsFinish true)
        (CallFunction|CancelingDrag)
        (Collision|SetCollisionProfileName (Variables|Default|GetStaticMesh) "TRICKignore" true :!class /Script/Engine.PrimitiveComponent)
        (Audio|SpawnSoundAttached "/Game/Project/Audio/MetaSoundSource/SE/MSS_S0003_CoverFinish.MSS_S0003_CoverFinish" (Variables|Default|GetSlideBarPivot) "None" "0, 0, 0" "0, 0, 0" "KeepRelativeOffset" false 1.0 1.0 0.0 0 0)
        (Variables|Default|SetbSoundPlaying false)
        (Variables|Default|SetbSliderLockOn true)
        (Variables|/Game/Project/Test/Prototype/BP_GlassCalculateMachine_V.BP_GlassCalculateMachine_V_C|SetbDrawerIsAuto _ref_calculatemachine true)
        (Variables|/Game/Project/Test/Prototype/BP_GlassCalculateMachine_V.BP_GlassCalculateMachine_V_C|SetbIsAutoOpen _ref_calculatemachine true)))))

(fn CheckSliderState
  (if (Variables|Default|GetbIsDraggingSlider)
    (if (Variables|Default|GetbHasUpdateMousePivot)
      (CallFunction|DragSliderViaInput)
      (else
        (Variables|Default|SetbHasUpdateMousePivot true)
        (CallFunction|UpdateTriggerMousePivot)))
    (elif (<= (.roll (Variables|/Script/Engine.SceneComponent|GetRelativeRotation (Variables|Default|GetSlideBarPivot))) -6e+01)
      (if (Variables|Default|GetbSliderLockOn)
        (CallFunction|SliderBacktoDefault)
        (else
          (CallFunction|FinishRemainingAngleCover)))
      (else
        (CallFunction|SliderBacktoDefault)))))

(fn DragSliderViaInput
  (bind _returnvalue (Game|GetPlayerController 0))
  (bind _triggermousepivot (Variables|Default|GetTriggerMousePivot))
  (bind _worldlocation (Game|Player|ConvertMouseLocationToWorldSpace _returnvalue))
  (bind _screenlocation (Class|PlayerController|ProjectWorldLocationtoScreen _returnvalue _worldlocation false))
  (if (not (Variables|Default|GetbSlideBarIsFinish))
    (if (!= (.y _screenlocation) (.y _triggermousepivot))
      (if (> (.y _screenlocation) (.y _triggermousepivot))
        (if (>= (.roll (Variables|/Script/Engine.SceneComponent|GetRelativeRotation (Variables|Default|GetSlideBarPivot))) -75.0)
          (Transformation|AddLocalRotation (Variables|Default|GetSlideBarPivot) (Math|Rotator|MakeRotator (* (Variables|Default|GetRotateSpeed) -1.0) 0.0 0.0) false false)
          (bind _output_get (Variables|Default|SetGearStartTime (* (Variables|Default|GetGearDuration) (/ (.roll (Variables|/Script/Engine.SceneComponent|GetRelativeRotation (Variables|Default|GetSlideBarPivot))) -75.0))))
          (Class|GeometryCacheComponent|SetStartTimeOffset (Variables|Default|GetGear) _output_get)
          (if (<= (.roll (Variables|/Script/Engine.SceneComponent|GetRelativeRotation (Variables|Default|GetSlideBarPivot))) -75.0)
            (Transformation|SetRelativeRotation (Variables|Default|GetSlideBarPivot) "0.000000,0.000000,-75.000000" false false)
            (else
              (CallFunction|UpdateTriggerMousePivot)
              (if (not (Variables|Default|GetbSoundPlaying))
                (Variables|Default|SetbSoundPlaying true)
                (Audio|SpawnSoundAttached "/Game/Project/Audio/MetaSoundSource/SE/MSS_S0003_CoverSlide.MSS_S0003_CoverSlide" (Variables|Default|GetSlideBarPivot) "None" "0, 0, 0" "0, 0, 0" "KeepRelativeOffset" false 1.0 1.0 0.0 0 0)))))))))

(fn SliderBacktoDefault
  (bind _slidebarpivot (Variables|Default|GetSlideBarPivot))
  (bind _slidebarpivot_2 (Variables|Default|GetSlideBarPivot))
  (bind _relativerotation (Variables|/Script/Engine.SceneComponent|GetRelativeRotation _slidebarpivot_2))
  (bind _relativerotation_2 (Variables|/Script/Engine.SceneComponent|GetRelativeRotation _slidebarpivot))
  (Utilities|FlowControl|Sequence
    (:then_0
      (Transformation|SetRelativeRotation (Variables|Default|GetSlideBarPivot) (Math|Interpolation|RInterpTo (Variables|/Script/Engine.SceneComponent|GetRelativeRotation (Variables|Default|GetSlideBarPivot)) (Math|Rotator|MakeRotator 0.0 (.pitch _relativerotation) (.yaw _relativerotation)) (Utilities|Time|GetWorldDeltaSeconds) 4.0) false false)
      (bind _output_get (Variables|Default|SetGearStartTime (* (Variables|Default|GetGearDuration) (/ (.roll (Variables|/Script/Engine.SceneComponent|GetRelativeRotation (Variables|Default|GetSlideBarPivot))) -75.0))))
      (Class|GeometryCacheComponent|SetStartTimeOffset (Variables|Default|GetGear) _output_get))
    (:then_1
      (if (>= (.roll (Variables|/Script/Engine.SceneComponent|GetRelativeRotation (Variables|Default|GetSlideBarPivot))) -1.0)
        (Transformation|SetRelativeRotation (Variables|Default|GetSlideBarPivot) (Math|Rotator|MakeRotator 0.0 (.pitch _relativerotation_2) (.yaw _relativerotation_2)) false false)
        (Collision|SetCollisionProfileName (Variables|Default|GetStaticMesh) "TRICKignore" true :!class /Script/Engine.PrimitiveComponent)
        (if (Variables|Default|GetbSlideBarIsFinish)
          (Audio|SpawnSoundAttached "/Game/Project/Audio/MetaSoundSource/SE/MSS_S0003_CoverFinish.MSS_S0003_CoverFinish" (Variables|Default|GetSlideBarPivot) "None" "0, 0, 0" "0, 0, 0" "KeepRelativeOffset" false 1.0 1.0 0.0 0 0)
          (Variables|Default|SetbSoundPlaying false)
          (Variables|Default|SetbSlideBarIsFinish false)
          (else
            (Variables|Default|SetbSliderLockOn false)))))))

(fn GearPreset
  (params (Gear :type Geometry%20Cache%20Component%20Object%20Reference) (Duration :type Float%20%28double-precision%29))
  (Variables|Default|SetGear Gear)
  (Variables|Default|SetGearDuration Duration))