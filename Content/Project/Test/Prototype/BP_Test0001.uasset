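; Prototype interactable door that swings open and closed and can be locked behind a match code.
; After a short delay, Interact uses a FlipFlop to play or reverse a rotation Timeline on the door mesh, provided it is unlocked or needs no object.
; InteractiveUnlocked clears the lock when the supplied code matches the configured one, with debug prints as feedback.
; Sound effects are still marked as pending.
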(event Custom|AnimPlay_CloseDoor
  ;[0.05098 0.05098 0.05098] Door Animation
  (bind _doortrack (Timeline|Timeline Reverse)
    (:Update
      (Transformation|SetRelativeRotation (Variables|Default|GetSM_Door) (Math|Rotator|MakeRotator _doortrack 9e+01 0.0) false false))))

(event Custom|AnimPlay_OpenDoor
  ;[0.05098 0.05098 0.05098] Door Animation
  (bind _doortrack (Timeline|Timeline Play)
    (:Update
      (Transformation|SetRelativeRotation (Variables|Default|GetSM_Door) (Math|Rotator|MakeRotator _doortrack 9e+01 0.0) false false))))

(event EventBeginPlay
  (|CallParentFunction)
  (bind _asbp_first_person_character (Utilities|Casting|CastToBP_FirstPersonCharacter (Game|GetPlayerCharacter 0)))
  (Variables|Default|SetPlayer _asbp_first_person_character))

(event EventInteract
  (params (InteractActor :type Actor%20Object%20Reference) (InteractTarget :type Actor%20Component%20Object%20Reference))
  ;[0.05098 0.05098 0.05098] Interact
  (Utilities|FlowControl|Delay 0.2)
  (if (or (Variables|Default|GetbInteractWithoutOBJ) (not (Variables|Default|GetbSTANDIsLocked)))
    (Utilities|FlowControl|FlipFlop
      (:A
        (CallFunction|AnimPlayOpenDoor))
      (:B
        (CallFunction|AnimPlayCloseDoor)))))

(event EventInteractiveUnlocked
  (params (MatchOBJCode :type Name :default "None"))
  ;[0.05098 0.05098 0.05098] CheckUnlockState
  (if (Variables|Default|GetbSTANDIsLocked)
    (if (Utilities|Enum|Equal(Enum) (Utilities|String|ToString(Name) MatchOBJCode) (Utilities|String|ToString(Name) (Variables|Default|GetSETMatchCode)))
      (Variables|Default|SetbSTANDIsLocked false)
      (Development|PrintString "Door Unlock!"))
    (else
      (Development|PrintString "Door Already Unlock"))))

(fn ConstructionScript
  (|CallParentFunction))