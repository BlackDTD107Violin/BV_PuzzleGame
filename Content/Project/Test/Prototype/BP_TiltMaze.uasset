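; BP_TiltMaze is a tilt-maze prototype actor that the player zooms into and out of.
; On BeginPlay it caches the first-person character and its BP_TiltMazeSET child actor, whose tick starts disabled.
; Zoomin blends the view to the maze, ignores move and look input, clears the prompt UI, switches mesh collision and enables the child's tick.
; ZoomOut returns the view and input, restores collision and stops that tick.
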(event EventBeginPlay
  (|CallParentFunction)
  (bind _asbp_first_person_character (Utilities|Casting|CastToBP_FirstPersonCharacter (Game|GetPlayerCharacter 0)))
  (Variables|Default|SetPlayer _asbp_first_person_character)
  (bind _asbp_tilt_maze_set (Utilities|Casting|CastToBP_TiltMazeSET (Variables|/Script/Engine.ChildActorComponent|GetChildActor (Variables|Default|GetChildActor))))
  (Variables|Default|SetChildActorREF _asbp_tilt_maze_set)
  (Actor|Tick|SetActorTickEnabled (Variables|Default|GetChildActorREF)))

(event EventZoomin
  (params (ZoomComponent :type Actor%20Component%20Object%20Reference))
  (bind _returnvalue (Game|GetPlayerController 0))
  (Game|Player|SetViewTargetwithBlend (Game|GetPlayerController 0) self 0.5 "VTBlend_Linear" 0.0 true)
  (Input|SetIgnoreMoveInput _returnvalue true)
  (Input|SetIgnoreLookInput _returnvalue true)
  (Default|ClearGamePromptUIView (Variables|Default|GetPlayer))
  (Collision|SetCollisionProfileName (Variables|Default|GetStaticMesh) "TRICKignore" true :!class /Script/Engine.PrimitiveComponent)
  (Actor|Tick|SetActorTickEnabled (Variables|Default|GetChildActorREF) true))

(event EventZoomOut
  (bind _returnvalue (Game|GetPlayerController 0))
  (Game|Player|SetViewTargetwithBlend (Game|GetPlayerController 0) (Game|GetPlayerCharacter 0) 0.5 "VTBlend_Linear" 0.0 true)
  (Input|ResetIgnoreMoveInput _returnvalue)
  (Input|ResetIgnoreLookInput _returnvalue)
  (Collision|SetCollisionProfileName (Variables|Default|GetStaticMesh) "BlockAllDynamic" true :!class /Script/Engine.PrimitiveComponent)
  (Actor|Tick|SetActorTickEnabled (Variables|Default|GetChildActorREF)))

(fn ConstructionScript
  (|CallParentFunction))