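; Mouse-draggable slider bar, a child actor of a glass mix or extract machine, that triggers its parent's merge or extract check when fully pulled.
; Tick turns vertical mouse movement into pivot roll while dragging; on release it eases to completion past a threshold, otherwise back to rest.
; A finished bar automatically returns to default, with slide and finish sounds.
; Zoomin/ZoomOut blend the view to and from this actor, toggling player move/look input.
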(event OnClicked(SlideBar)
  (params (TouchedComponent :type Primitive%20Component%20Object%20Reference) (ButtonPressed :type Key%20Structure))
  (if (Variables|Default|GetbSlideBarIsFinish)
    (Variables|Default|SetbIsDraggingSlider false)
    (else
      (Variables|Default|SetbIsDraggingSlider true)
      (Variables|/Game/ProjectDefault/FirstPerson/Blueprints/BP_FirstPersonCharacter.BP_FirstPersonCharacter_C|SetCurrentInteract (Variables|Default|GetPlayer_0) self))))

(event EventBeginPlay
  (bind _returnvalue (Game|GetPlayerController 0))
  (|CallParentFunction)
  (bind _asbp_first_person_character (Utilities|Casting|CastToBP_FirstPersonCharacter (Game|GetPlayerCharacter 0)))
  (Variables|Default|SetPlayer_0 _asbp_first_person_character)
  (Input|EnableInput _returnvalue)
  (Variables|/Script/Engine.PlayerController|SetbEnableClickEvents _returnvalue true)
  (Variables|/Script/Engine.PlayerController|SetbEnableMouseOverEvents _returnvalue true)
  (bind _asbp_glass_mix_machine (Utilities|Casting|CastToBP_GlassMixMachine (Actor|GetParentActor))
    (:then
      (Variables|Default|SetREF_GlassMixMachine _asbp_glass_mix_machine))
    (:CastFailed
      (bind _asbp_extract_machine (Utilities|Casting|CastToBP_ExtractMachine (Actor|GetParentActor)))
      (Variables|Default|SetREF_ExtractMachine _asbp_extract_machine)
      (Variables|Default|SetbIsExtractMachine true))))

(event EventTick
  (params (DeltaSeconds :type Float%20%28single-precision%29))
  (if (Variables|Default|GetbSlideBarIsFinish)
    (CallFunction|SliderBacktoDefault)
    (else
      (CallFunction|CheckSliderState))))

(event EventZoomin
  (params (ZoomComponent :type Actor%20Component%20Object%20Reference))
  (bind _returnvalue (Game|GetPlayerController 0))
  (Game|Player|SetViewTargetwithBlend (Game|GetPlayerController 0) self 0.5 "VTBlend_Linear" 0.0 true)
  (Input|SetIgnoreMoveInput _returnvalue true)
  (Input|SetIgnoreLookInput _returnvalue true)
  (Default|ClearGamePromptUIView (Variables|Default|GetPlayer_0))
  (Collision|SetCollisionProfileName (Variables|Default|GetZoomTrigger_Main) "NoCollision" true :!class /Script/Engine.PrimitiveComponent))

(event EventZoomOut
  (bind _returnvalue (Game|GetPlayerController 0))
  (Game|Player|SetViewTargetwithBlend (Game|GetPlayerController 0) (Game|GetPlayerCharacter 0) 0.5 "VTBlend_Linear" 0.0 true)
  (Input|ResetIgnoreMoveInput _returnvalue)
  (Input|ResetIgnoreLookInput _returnvalue)
  (Utilities|FlowControl|Delay 0.5)
  (Collision|SetCollisionProfileName (Variables|Default|GetZoomTrigger_Main) "BlockAllDynamic" true :!class /Script/Engine.PrimitiveComponent))

(event EventInteractEnd
  (CallFunction|CancelingDrag)
  (Variables|/Game/ProjectDefault/FirstPerson/Blueprints/BP_FirstPersonCharacter.BP_FirstPersonCharacter_C|SetCurrentInteract (Variables|Default|GetPlayer_0) self)
  (Variables|Default|SetbSoundPlaying false))

(fn ConstructionScript
  (|CallParentFunction))

(fn UpdateTriggerMousePivot
  (bind _returnvalue (Game|GetPlayerController 0))
  (Variables|Default|SetTriggerMousePivot (.ScreenLocation (Class|PlayerController|ProjectWorldLocationtoScreen _returnvalue (.WorldLocation (Game|Player|ConvertMouseLocationToWorldSpace _returnvalue)) false))))

(fn CancelingDrag
  (Variables|Default|SetbIsDraggingSlider false)
  (Variables|Default|SetbHasUpdateMousePivot false))

(fn FinishRemainingAngleCover
  (bind _slidebarpivot (Variables|Default|GetSlideBarPivot))
  (bind _slidebarpivot_2 (Variables|Default|GetSlideBarPivot))
  (bind _relativerotation (Variables|/Script/Engine.SceneComponent|GetRelativeRotation _slidebarpivot))
  (bind _relativerotation_2 (Variables|/Script/Engine.SceneComponent|GetRelativeRotation _slidebarpivot_2))
  (Utilities|FlowControl|Sequence
    (:then_0
      (Transformation|SetRelativeRotation (Variables|Default|GetSlideBarPivot) (Math|Interpolation|RInterpTo (Variables|/Script/Engine.SceneComponent|GetRelativeRotation (Variables|Default|GetSlideBarPivot)) (Math|Rotator|MakeRotator -75.0 (.pitch _relativerotation) (.yaw _relativerotation)) (Utilities|Time|GetWorldDeltaSeconds) 4.0) false false))
    (:then_1
      (if (<= (.roll (Variables|/Script/Engine.SceneComponent|GetRelativeRotation (Variables|Default|GetSlideBarPivot))) -74.0)
        (Transformation|SetRelativeRotation (Variables|Default|GetSlideBarPivot) (Math|Rotator|MakeRotator -75.0 (.pitch _relativerotation_2) (.yaw _relativerotation_2)) false false)
        (Variables|Default|SetbSlideBarIsFinish true)
        (if (Variables|Default|GetbIsExtractMachine)
          (Default|CheckExtractRequest (Variables|Default|GetREF_ExtractMachine))
          (else
            (Default|CheckMergeRequest (Variables|Default|GetREF_GlassMixMachine))))
        (CallFunction|CancelingDrag)
        (Collision|SetCollisionProfileName (Variables|Default|GetStaticMesh) "TRICKignore" true :!class /Script/Engine.PrimitiveComponent)
        (Audio|SpawnSoundAttached "/Game/Project/Audio/MetaSoundSource/SE/MSS_S0003_CoverFinish.MSS_S0003_CoverFinish" (Variables|Default|GetSlideBarPivot) "None" "0, 0, 0" "0, 0, 0" "KeepRelativeOffset" false 1.0 1.0 0.0 0 0)
        (Variables|Default|SetbSoundPlaying false)))))

(fn CheckSliderState
  (if (Variables|Default|GetbIsDraggingSlider)
    (if (Variables|Default|GetbHasUpdateMousePivot)
      (CallFunction|DragSliderViaInput)
      (else
        (Variables|Default|SetbHasUpdateMousePivot true)
        (CallFunction|UpdateTriggerMousePivot)))
    (elif (<= (.roll (Variables|/Script/Engine.SceneComponent|GetRelativeRotation (Variables|Default|GetSlideBarPivot))) -6e+01)
      (CallFunction|FinishRemainingAngleCover)
      (else
        (CallFunction|SliderBacktoDefault)))))

(fn DragSliderViaInput
  (bind _returnvalue (Game|GetPlayerController 0))
  (bind _triggermousepivot (Variables|Default|GetTriggerMousePivot))
  (bind _worldlocation (Game|Player|ConvertMouseLocationToWorldSpace _returnvalue))
  (bind _screenlocation (Class|PlayerController|ProjectWorldLocationtoScreen _returnvalue _worldlocation false))
  (if (not (Variables|Default|GetbSlideBarIsFinish))
    (if (!= (.y _screenlocation) (.y _triggermousepivot))
      (if (> (.y _screenlocation) (.y _triggermousepivot))
        (Transformation|AddLocalRotation (Variables|Default|GetSlideBarPivot) (Math|Rotator|MakeRotator (* (Variables|Default|GetRotateSpeed) -1.0) 0.0 0.0) false false)
        (if (>= (.roll (Variables|/Script/Engine.SceneComponent|GetRelativeRotation (Variables|Default|GetSlideBarPivot))) 0.0)
          (Transformation|SetRelativeRotation (Variables|Default|GetSlideBarPivot) "0, 0, 0" false false)
          (else
            (CallFunction|UpdateTriggerMousePivot)
            (if (not (Variables|Default|GetbSoundPlaying))
              (Variables|Default|SetbSoundPlaying true)
              (Audio|SpawnSoundAttached "/Game/Project/Audio/MetaSoundSource/SE/MSS_S0003_CoverSlide.MSS_S0003_CoverSlide" (Variables|Default|GetSlideBarPivot) "None" "0, 0, 0" "0, 0, 0" "KeepRelativeOffset" false 1.0 1.0 0.0 0 0))))
        (else
          (Transformation|AddLocalRotation (Variables|Default|GetSlideBarPivot) (Math|Rotator|MakeRotator (Variables|Default|GetRotateSpeed) 0.0 0.0) false false)
          (if (<= (Class|KismetMathLibrary|ClampAxis (.roll (Variables|/Script/Engine.SceneComponent|GetRelativeRotation (Variables|Default|GetSlideBarPivot)))) 2.7e+02)
            (Variables|Default|SetbSlideBarIsFinish true)
            (if (Variables|Default|GetbIsExtractMachine)
              (Default|CheckExtractRequest (Variables|Default|GetREF_ExtractMachine))
              (else
                (Default|CheckMergeRequest (Variables|Default|GetREF_GlassMixMachine))))
            (CallFunction|CancelingDrag)
            (Collision|SetCollisionProfileName (Variables|Default|GetStaticMesh) "TRICKignore" true :!class /Script/Engine.PrimitiveComponent)
            (Audio|SpawnSoundAttached "/Game/Project/Audio/MetaSoundSource/SE/MSS_S0003_CoverFinish.MSS_S0003_CoverFinish" (Variables|Default|GetSlideBarPivot) "None" "0, 0, 0" "0, 0, 0" "KeepRelativeOffset" false 1.0 1.0 0.0 0 0)
            (Variables|Default|SetbSoundPlaying false)
            (else
              (CallFunction|UpdateTriggerMousePivot)
              (if (not (Variables|Default|GetbSoundPlaying))
                (Variables|Default|SetbSoundPlaying true)
                (Audio|SpawnSoundAttached "/Game/Project/Audio/MetaSoundSource/SE/MSS_S0003_CoverSlide.MSS_S0003_CoverSlide" (Variables|Default|GetSlideBarPivot) "None" "0, 0, 0" "0, 0, 0" "KeepRelativeOffset" false 1.0 1.0 0.0 0 0)))))))))

(fn SliderBacktoDefault
  (bind _slidebarpivot (Variables|Default|GetSlideBarPivot))
  (bind _slidebarpivot_2 (Variables|Default|GetSlideBarPivot))
  (bind _relativerotation (Variables|/Script/Engine.SceneComponent|GetRelativeRotation _slidebarpivot_2))
  (bind _relativerotation_2 (Variables|/Script/Engine.SceneComponent|GetRelativeRotation _slidebarpivot))
  (Utilities|FlowControl|Sequence
    (:then_0
      (Transformation|SetRelativeRotation (Variables|Default|GetSlideBarPivot) (Math|Interpolation|RInterpTo (Variables|/Script/Engine.SceneComponent|GetRelativeRotation (Variables|Default|GetSlideBarPivot)) (Math|Rotator|MakeRotator 0.0 (.pitch _relativerotation) (.yaw _relativerotation)) (Utilities|Time|GetWorldDeltaSeconds) 4.0) false false))
    (:then_1
      (if (>= (.roll (Variables|/Script/Engine.SceneComponent|GetRelativeRotation (Variables|Default|GetSlideBarPivot))) -1.0)
        (Transformation|SetRelativeRotation (Variables|Default|GetSlideBarPivot) (Math|Rotator|MakeRotator 0.0 (.pitch _relativerotation_2) (.yaw _relativerotation_2)) false false)
        (Collision|SetCollisionProfileName (Variables|Default|GetStaticMesh) "TRICKignore" true :!class /Script/Engine.PrimitiveComponent)
        (if (Variables|Default|GetbSlideBarIsFinish)
          (Audio|SpawnSoundAttached "/Game/Project/Audio/MetaSoundSource/SE/MSS_S0003_CoverFinish.MSS_S0003_CoverFinish" (Variables|Default|GetSlideBarPivot) "None" "0, 0, 0" "0, 0, 0" "KeepRelativeOffset" false 1.0 1.0 0.0 0 0)
          (Variables|Default|SetbSoundPlaying false)
          (Variables|Default|SetbSlideBarIsFinish false))))))