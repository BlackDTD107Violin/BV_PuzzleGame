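; Prototype draggable chair that the first-person player can hold and swing around while interacting, with an optional lock cleared by a matching object code.
; Interact records half the player distance, applies a mass-based speed penalty, switches collision to the drag component and enables Tick.
; Tick eases the chair, with sweep, toward that radius along the player's yaw and turns its mesh.
; InteractEnd stops Tick and restores blocking collision.
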(event EventBeginPlay
  (|CallParentFunction)
  (bind _asbp_first_person_character (Utilities|Casting|CastToBP_FirstPersonCharacter (Game|GetPlayerCharacter 0)))
  (Variables|Default|SetPlayer%20REF _asbp_first_person_character)
  (Collision|SetCollisionEnabled (Variables|Default|GetDragCollision) "NoCollision"))

(event EventTick
  (params (DeltaSeconds :type Float%20%28single-precision%29))
  (CallFunction|RotateAroundPlayer (Variables|Default|GetDistance)))

(event EventInteract
  (params (InteractActor :type Actor%20Object%20Reference) (InteractTarget :type Actor%20Component%20Object%20Reference))
  (if (or (Variables|Default|GetbInteractWithoutOBJ) (not (Variables|Default|GetbSTANDIsLocked)))
    (Variables|Default|SetDistance (/ (Transformation|GetDistanceTo self (Variables|Default|GetPlayer%20REF)) 2.0))
    (Variables|/Game/ProjectDefault/FirstPerson/Blueprints/BP_FirstPersonCharacter.BP_FirstPersonCharacter_C|SetbIsPressed (Variables|Default|GetPlayer%20REF) true)
    (if (Variables|Default|GetbSETDraggable)
      (Actor|Tick|SetActorTickEnabled true)
      (Default|SpeedNerfViaDragSET (Variables|Default|GetPlayer%20REF) (Variables|Default|GetMass))
      (Collision|SetCollisionProfileName (Variables|Default|GetStaticMesh) "PawnIgnore" true :!class /Script/Engine.PrimitiveComponent)
      (Physics|SetSimulatePhysics (Variables|Default|GetDragCollision) true)
      (Collision|SetCollisionEnabled (Variables|Default|GetDragCollision) "QueryAndPhysics"))))

(event EventInteractiveUnlocked
  (params (MatchOBJCode :type Name :default "None"))
  (if (Variables|Default|GetbSTANDIsLocked)
    (if (Utilities|Enum|Equal(Enum) (Utilities|String|ToString(Name) MatchOBJCode) (Utilities|String|ToString(Name) (Variables|Default|GetSETMatchCode)))
      (Variables|Default|SetbSTANDIsLocked false))))

(event EventInteractEnd
  (Variables|/Game/ProjectDefault/FirstPerson/Blueprints/BP_FirstPersonCharacter.BP_FirstPersonCharacter_C|SetbIsPressed (Variables|Default|GetPlayer%20REF) false)
  (Actor|Tick|SetActorTickEnabled false)
  (Collision|SetCollisionProfileName (Variables|Default|GetStaticMesh) "BlockAllDynamic" true :!class /Script/Engine.PrimitiveComponent)
  (Collision|SetCollisionEnabled (Variables|Default|GetDragCollision) "NoCollision"))

(fn ConstructionScript
  (|CallParentFunction))

(fn UpdatePosViaPlayerInput
  (bind _player_ref (Variables|Default|GetPlayer%20REF))
  (bind _gapbetweenplayer (Variables|Default|GetGapBetweenPlayer))
  (bind _returnvalue (Transformation|GetActorLocation _player_ref))
  (bind _returnvalue_2 (+ _returnvalue _gapbetweenplayer))
  (Transformation|SetActorLocation (Math|Vector|MakeVector (.x _returnvalue_2) (.y _returnvalue_2) (.z (Transformation|GetActorLocation self))) false false))

(fn UpdateDirViaPlayerInput
  (Transformation|SetActorRotation (Math|Rotator|MakeRotator 0.0 0.0 (.yaw (Transformation|GetActorRotation (Variables|Default|GetPlayer%20REF))))))

(fn RotateAroundPlayer
  (params (Radius :type Float%20%28double-precision%29))
  (bind _returnvalue (Math|Vector|MakeVector Radius 0.0 0.0))
  (bind _returnvalue_2 (Game|GetPlayerCharacter 0))
  (bind _player_ref (Variables|Default|GetPlayer%20REF))
  (bind _returnvalue_3 (Transformation|GetActorRotation _player_ref))
  (bind _returnvalue_4 (Transformation|GetActorLocation _returnvalue_2))
  (bind _returnvalue_5 (Math|Vector|RotateVectorAroundAxis _returnvalue (.yaw _returnvalue_3) "0.000000,0.000000,1.000000"))
  (Transformation|SetActorLocation (Math|Interpolation|VInterpTo (Transformation|GetActorLocation self) (Math|Vector|MakeVector (+ (.x _returnvalue_4) (.x _returnvalue_5)) (+ (.y _returnvalue_4) (.y _returnvalue_5)) (.z _returnvalue_5)) 15.0 0.01) true false)
  (Transformation|SetWorldRotation (Variables|Default|GetStaticMesh) (Math|Rotator|MakeRotator 0.0 0.0 (+ (.yaw (Transformation|GetActorRotation (Variables|Default|GetPlayer%20REF))) 9e+01)) false false))