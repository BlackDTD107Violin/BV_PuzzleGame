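; Prototype gear interaction actor that links a child slider bar to a gear and offers a zoomed-in view for using it.
; On BeginPlay it caches the first-person character, enables input with mouse click and hover events, and passes the gear and its duration to the slider.
; Zoom events blend the camera to or from the actor, toggle player move and look input, and switch the zoom trigger's collision.
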(event EventBeginPlay
  (bind _returnvalue (Game|GetPlayerController 0))
  (bind _gear (Variables|Default|GetGear))
  (|CallParentFunction)
  (bind _asbp_first_person_character (Utilities|Casting|CastToBP_FirstPersonCharacter (Game|GetPlayerCharacter 0)))
  (Variables|Default|SetPlayer_0 _asbp_first_person_character)
  (Input|EnableInput _returnvalue)
  (Variables|/Script/Engine.PlayerController|SetbEnableClickEvents _returnvalue true)
  (Variables|/Script/Engine.PlayerController|SetbEnableMouseOverEvents _returnvalue true)
  (bind _asbp_gear_slider_bar (Utilities|Casting|CastToBP_GearSliderBar (Variables|/Script/Engine.ChildActorComponent|GetChildActor (Variables|Default|GetSlider))))
  (Default|GearPreset _asbp_gear_slider_bar _gear (Media|MediaPlayer|GetDuration _gear)))

(event EventZoomin
  (params (ZoomComponent :type Actor%20Component%20Object%20Reference))
  (bind _returnvalue (Game|GetPlayerController 0))
  (Game|Player|SetViewTargetwithBlend (Game|GetPlayerController 0) self 0.5 "VTBlend_Linear" 0.0 true)
  (Input|SetIgnoreMoveInput _returnvalue true)
  (Input|SetIgnoreLookInput _returnvalue true)
  (Default|ClearGamePromptUIView (Variables|Default|GetPlayer_0))
  (Collision|SetCollisionProfileName (Variables|Default|GetZoomTrigger_Main) "NoCollision" true :!class /Script/Engine.PrimitiveComponent)
  (if (> (Utilities|Array|Length (Variables|Default|GetChildLists)) 0)
    _))

(event EventZoomOut
  (bind _returnvalue (Game|GetPlayerController 0))
  (Game|Player|SetViewTargetwithBlend (Game|GetPlayerController 0) (Game|GetPlayerCharacter 0) 0.5 "VTBlend_Linear" 0.0 true)
  (Input|ResetIgnoreMoveInput _returnvalue)
  (Input|ResetIgnoreLookInput _returnvalue)
  (Utilities|FlowControl|Delay 0.5)
  (Collision|SetCollisionProfileName (Variables|Default|GetZoomTrigger_Main) "BlockAllDynamic" true :!class /Script/Engine.PrimitiveComponent))

(fn ConstructionScript
  (|CallParentFunction))