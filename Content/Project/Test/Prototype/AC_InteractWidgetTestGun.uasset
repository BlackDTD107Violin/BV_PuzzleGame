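; Prototype test gun interactable, apparently intended as a pickup with an on-screen interact prompt.
; Currently Interact is empty and ShowPromptSET only checks flags without acting, while ShowPrompt just destroys the actor.
; Disconnected logic holds the intended flow: creating and removing the widget, toggling its pressed state, and adding a weapon component to the first-person character before destroying the pickup.
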(event EventInteract
  (params (InteractTarget :type Actor%20Component%20Object%20Reference))
  ;[0.05098 0.05098 0.05098] Interact
)

(event EventShowPromptSET
  (params (bIsShow :type Boolean))
  ;[0.05098 0.05098 0.05098] Widget_IO_according to the player is in the Trigger Area or not
  (if bIsShow
    (if (Variables|Default|GetbIsExist)
      _)))

(fn ConstructionScript)