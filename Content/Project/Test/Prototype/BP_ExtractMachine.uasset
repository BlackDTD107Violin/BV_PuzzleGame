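; BP_ExtractMachine is a prototype machine that extracts data from an inserted object and creates the result in a mix glass notch.
; On BeginPlay it registers itself with its child slider bar and caches the child-actor input and output notches, passing the glass pool to the output.
; CheckExtractRequest forwards stored extract data to the output notch only when an object is set, no extraction is running and that notch is empty, otherwise printing debug messages.
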(event EventBeginPlay
  (|CallParentFunction)
  (Utilities|FlowControl|Sequence
    (:then_0
      (bind _asbp_mix_machine_slider_bar (Utilities|Casting|CastToBP_MixMachineSliderBar (Variables|/Script/Engine.ChildActorComponent|GetChildActor (Variables|Default|GetSliderBar))))
      (Variables|/Game/Project/Test/Prototype/BP_MixMachineSliderBar.BP_MixMachineSliderBar_C|SetREF_ExtractMachine _asbp_mix_machine_slider_bar self)
      (Variables|/Game/Project/Test/Prototype/BP_MixMachineSliderBar.BP_MixMachineSliderBar_C|SetbIsExtractMachine _asbp_mix_machine_slider_bar true))
    (:then_1
      (CallFunction|PresetEachNotch))))

(fn ConstructionScript
  (|CallParentFunction))

(fn CheckExtractRequest
  (if (Math|Boolean|ANDBoolean (Variables|Default|GetbOBJNotchIsSet) (not (Variables|Default|GetbIsExtracting)) (Variables|Default|GetbMixNotchIsEmpty))
    (Default|ReceiveExtractDataandCreate (Variables|Default|GetOutput%20Notch) (.ExtractData (Utilities|Struct|BreakST_ItemCollection (Variables|Default|GetOBJExtractData))))
    (Variables|Default|SetbMixNotchIsEmpty false)
    (elif (Variables|Default|GetbIsExtracting)
      (Development|PrintString "During Extracting")
      (elif (Variables|Default|GetbMixNotchIsEmpty)
        (Development|PrintString "OBJ Notch Is Empty")
        (else
          (Development|PrintString "Mix Notch Has Glass"))))))

(fn PresetEachNotch
  (Utilities|FlowControl|Sequence
    (:then_0
      (bind _asbp_glassnotch_extract (Utilities|Casting|CastToBP_GLASSnotch_Extract (Variables|/Script/Engine.ChildActorComponent|GetChildActor (Variables|Default|GetExtractNotch))))
      (Variables|Default|SetOBJInputNotch _asbp_glassnotch_extract))
    (:then_1
      (bind _asbp_glassnotch_mix (Utilities|Casting|CastToBP_GLASSnotch_Mix (Variables|/Script/Engine.ChildActorComponent|GetChildActor (Variables|Default|GetGLASSNotch_Mix))))
      (bind _output_get (Variables|Default|SetOutput%20Notch _asbp_glassnotch_mix))
      (Default|SetupGlassTAside _output_get "NewEnumerator3")
      (Variables|/Game/Project/Test/Prototype/BP_GLASSnotch_Mix.BP_GLASSnotch_Mix_C|SetREF_GlassPool (Variables|Default|GetOutput%20Notch) (Variables|Default|GetREF_GlassPool)))))

(fn ReceiveOBJExtractCode
  (params (InsertedOBJ :type ST%20Item%20Collection%20Structure))
  (Variables|Default|SetOBJExtractData InsertedOBJ)
  (Variables|Default|SetbOBJNotchIsSet true))