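; BP_Chalice is a placeable pickup that shows interact and pick-up prompt widgets and exposes key serial and extract codes.
; It records its starting transform on BeginPlay; SetTempPos stores an offset transform and parent, flip-flopping a drawer open/closed flag on each call.
; Repos restores the temporary or original transform based on that flag, then reattaches to the parent.
; Its Pickup and Interact events are empty.
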(event EventBeginPlay
  (Variables|Default|SetOriginalPos (Transformation|GetActorTransform)))

(event EventSetTempPos
  (params (TempPos :type Vector :default "0, 0, 0") (Parent :type Static%20Mesh%20Component%20Object%20Reference))
  (bind _originalpos (Variables|Default|GetOriginalPos))
  (Variables|Default|SetReAttach Parent)
  (Variables|Default|SetTempPos (Math|Transform|MakeTransform (+ TempPos (.location _originalpos)) (.rotation _originalpos) (.scale _originalpos)))
  (Utilities|FlowControl|FlipFlop
    (:A
      (Variables|Default|SetbTargetOnTemp true)
      (Development|PrintString "Drawer Open"))
    (:B
      (Variables|Default|SetbTargetOnTemp false)
      (Development|PrintString "Drawer Close"))))

(event EventPickup
  (params (InteractTarget :type Actor%20Component%20Object%20Reference)))

(event EventRepos
  (bind _reattach (Variables|Default|GetReAttach))
  (if (Variables|Default|GetbTargetOnTemp)
    (Transformation|SetActorRelativeTransform (Variables|Default|GetTempPos) false false)
    (Development|PrintString "Back to Temp Pos")
    (Transformation|AttachComponentToComponent _reattach "None" "KeepWorld" "KeepWorld" "KeepWorld" true)
    (else
      (Transformation|SetActorRelativeTransform (Variables|Default|GetOriginalPos) false false)
      (Development|PrintString "Back to Original Pos")
      (Transformation|AttachComponentToComponent _reattach "None" "KeepWorld" "KeepWorld" "KeepWorld" true))))

(event EventShowPromptInteract
  (params (bIsShow :type Boolean))
  ;[0.05098 0.05098 0.05098] Widget_IO_according to the player is in the Interact Trigger Area or not
  (if bIsShow
    (if (not (Variables|Default|GetbInteractPromptIsExist))
      (bind _returnvalue (UserInterface|CreateWidget "/Game/Developers/LinYanChen/WBP_InteractPrompt.WBP_InteractPrompt_C"))
      (UserInterface|Viewport|AddtoViewport _returnvalue 0)
      (Variables|Default|SetbInteractPromptIsExist true))
    (else
      (Widget|RemovefromParent _returnvalue)
      (Variables|Default|SetbInteractPromptIsExist false))))

(event EventShowPromptPick
  (params (bIsShow :type Boolean))
  ;[0.05098 0.05098 0.05098] Widget_IO_according to the player is in the Pickup Trigger Area or not
  (if bIsShow
    (if (not (Variables|Default|GetbPickPromptIsExist))
      (bind _returnvalue (UserInterface|CreateWidget "/Game/Developers/LinYanChen/WBP_PickPrompt.WBP_PickPrompt_C"))
      (UserInterface|Viewport|AddtoViewport _returnvalue 0)
      (Variables|Default|SetbPickPromptIsExist true))
    (else
      (Widget|RemovefromParent _returnvalue)
      (Variables|Default|SetbPickPromptIsExist false))))

(event EventInteract
  (params (InteractTarget :type Actor%20Component%20Object%20Reference)))

(fn ConstructionScript
  (|CallParentFunction))

(fn ReturnOBJCode
  (return (Variables|Default|GetKeySerialCode) (Variables|Default|GetExtractSerialCode)))