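; BP_Dagger is a dagger pickup that shows the ReadingP0001 readable on the tutorial player character when picked up.
; Events toggle its pickup and interact prompt widgets, though Interact is empty and SetupWidget is never called.
; Repos restores the original transform and, if parented, re-attaches to the root stored by SetTempPos at the key-code socket, reopens the reading, and fires a one-time tutorial arrival that clears the prompt UI.
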(event EventBeginPlay
  (CallFunction|SetupParent)
  (bind _asbp_first_person_character_tutorial (Utilities|Casting|CastToBP_FirstPersonCharacterTutorial (Game|GetPlayerCharacter 0)))
  (Variables|Default|SetPlayer _asbp_first_person_character_tutorial))

(event EventPickup
  (params (InteractTarget :type Actor%20Component%20Object%20Reference))
  (Default|InteractwithReadingOBJ (Variables|Default|GetPlayer) "ReadingP0001"))

(event EventRepos
  (bind _player (Variables|Default|GetPlayer))
  ;[0.05098 0.05098 0.05098] Set Actor Repos
  (Transformation|SetActorRelativeTransform (Variables|Default|GetOriginalPos) false false)
  (if (Variables|Default|GetbHasParent)
    (Transformation|AttachComponentToComponent (Variables|Default|GetReAttach) (Variables|Default|GetKeySerialCode) "SnapToTarget" "KeepWorld" "KeepWorld" true)
    (Default|InteractwithReadingOBJ (Variables|Default|GetPlayer) "ReadingP0001")
    (if (not (Variables|Default|GetbHasTriggerTutor))
      (Variables|Default|SetbHasTriggerTutor true)
      (Default|ArriveTutorialTA _player)
      (Default|ClearGamePromptUIView _player))))

(event EventSetTempPos
  (params (Root :type Static%20Mesh%20Component%20Object%20Reference))
  ;[0.05098 0.05098 0.05098] Set Actor Repos
  ;;[0.05098 0.05098 0.05098] Temp Repos will execute when the root parent is moving
  (Variables|Default|SetReAttach Root))

(event EventShowPromptInteract
  (params (bIsShow :type Boolean))
  (bind _ref_interactprompt (Variables|Default|GetREF_InteractPrompt))
  ;[0.05098 0.05098 0.05098] Widget_IO_according to the player is in the Interact Trigger Area or not
  (if bIsShow
    (Widget|SetVisibility _ref_interactprompt "Visible")
    (else
      (Widget|SetVisibility _ref_interactprompt "Hidden"))))

(event EventShowPromptPick
  (params (bIsShow :type Boolean))
  (bind _ref_pickprompt (Variables|Default|GetREF_PickPrompt))
  ;[0.05098 0.05098 0.05098] Widget_IO_according to the player is in the Pickup Trigger Area or not
  (if bIsShow
    (Widget|SetVisibility _ref_pickprompt "Visible")
    (else
      (Widget|SetVisibility _ref_pickprompt "Hidden"))))

(event EventInteract
  (params (InteractTarget :type Actor%20Component%20Object%20Reference)))

(fn ConstructionScript)

(fn ReturnOBJCode
  (return "None" 0))