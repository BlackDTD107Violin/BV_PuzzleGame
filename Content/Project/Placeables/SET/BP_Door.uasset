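; BP_Door is a placeable interactable door that toggles open and closed on each Interact.
; A FlipFlop alternates OpenDoor and CloseDoor, which play or reverse one Timeline driving the door mesh's relative roll.
; ShowPromptSET adds or removes an interact prompt widget, using a flag to prevent duplicate creation.
; Interact briefly sets the prompt's pressed state and waits for that short delay before the door moves.
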(event Custom|CloseDoor
  ;[0.05098 0.05098 0.05098] Door Animation
  (bind _doortrack (Timeline|Timeline Reverse)
    (:Update
      (Transformation|SetRelativeRotation (Variables|Default|GetSM_Door) (Math|Rotator|MakeRotator _doortrack 9e+01 0.0) false false))))

(event Custom|OpenDoor
  ;[0.05098 0.05098 0.05098] Door Animation
  (bind _doortrack (Timeline|Timeline Play)
    (:Update
      (Transformation|SetRelativeRotation (Variables|Default|GetSM_Door) (Math|Rotator|MakeRotator _doortrack 9e+01 0.0) false false))))

(event EventShowPromptSET
  (params (bIsShow :type Boolean))
  ;[0.05098 0.05098 0.05098] Widget_IO_according to the player is in the Trigger Area or not
  (if bIsShow
    (if (not (Variables|Default|GetbWidgetIsExist))
      (bind _returnvalue (UserInterface|CreateWidget "/Game/Developers/LinYanChen/WBP_InteractPrompt.WBP_InteractPrompt_C"))
      (UserInterface|Viewport|AddtoViewport _returnvalue 0)
      (Variables|Default|SetbWidgetIsExist true))
    (else
      (Widget|RemovefromParent _returnvalue)
      (Variables|Default|SetbWidgetIsExist false))))

(event EventInteract
  (params (InteractTarget :type Actor%20Component%20Object%20Reference))
  ;[0.05098 0.05098 0.05098] Interact
  (Variables|/Game/Developers/LinYanChen/WBP_InteractPrompt.WBP_InteractPrompt_C|SetIsPressed (stale EventShowPromptSET _returnvalue) true)
  (Utilities|FlowControl|Delay 0.2)
  (Variables|/Game/Developers/LinYanChen/WBP_InteractPrompt.WBP_InteractPrompt_C|SetIsPressed (stale EventShowPromptSET _returnvalue) false)
  (Utilities|FlowControl|FlipFlop
    (:A
      (CallFunction|OpenDoor))
    (:B
      (CallFunction|CloseDoor))))

(fn ConstructionScript
  (|CallParentFunction))