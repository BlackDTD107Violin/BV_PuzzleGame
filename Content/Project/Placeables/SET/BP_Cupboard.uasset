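; Interactive cupboard Blueprint that slides individual drawers open and closed and shows an interact prompt widget on request.
; Interact ignores the cupboard body and passes other meshes to DrawerFlipFlop, which picks the slide direction from the drawer's relative X.
; A Timeline lerps the drawer while CanOpen blocks re-entry, and actors found by the drawer's child-actor classes are messaged with that drawer.
; StandByFunc is an unfinished per-drawer state switch.
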(event Custom|StandByFunc
  (params (TargetName :type String))
  (switch string TargetName))

(event Custom|DrawerFlipFlop
  (params (SM_REF :type Static%20Mesh%20Component%20Object%20Reference))
  ;[0.05098 0.05098 0.05098] Interact
  ;;[0.05098 0.05098 0.05098] Check Drawer State then assign FlipFlop location
  (bind _output_get (Variables|Components|SetSM_REF SM_REF))
  (CallFunction|StandbyFunc (Utilities|String|ToString(Object) _output_get))
  (Variables|Default|SetStartLocation (Math|Vector|MakeVector (.x (Variables|/Script/Engine.SceneComponent|GetRelativeLocation _output_get)) (.y (Variables|/Script/Engine.SceneComponent|GetRelativeLocation _output_get)) (.z (Variables|/Script/Engine.SceneComponent|GetRelativeLocation _output_get))))
  (Variables|Default|SetEndLocation (Math|Vector|MakeVector (+ (.x (Variables|/Script/Engine.SceneComponent|GetRelativeLocation _output_get)) (Math|Float|SelectFloat 35.0 -35.0 (not (>= (.x (Variables|/Script/Engine.SceneComponent|GetRelativeLocation SM_REF)) 2e+01)))) (.y (Variables|/Script/Engine.SceneComponent|GetRelativeLocation _output_get)) (.z (Variables|/Script/Engine.SceneComponent|GetRelativeLocation _output_get))))
  (for _array_element (Components|GetChildrenComponents (Variables|Components|GetSM_REF) false)
    (bind _aschild_actor_component (Utilities|Casting|CastToChildActorComponent _array_element))
    (bind _returnvalue (Actor|GetActorOfClass (Variables|/Script/Engine.ChildActorComponent|GetChildActorClass _aschild_actor_component)))
    (Class|BIOBJInteractInterface|SetTempPos2(Message) _returnvalue (Variables|Components|GetSM_REF))))

(event EventInteract
  (params (InteractTarget :type Actor%20Component%20Object%20Reference))
  ;[0.05098 0.05098 0.05098] Interact
  (if (Variables|Default|GetbCanOpen)
    (Variables|Default|SetbCanOpen false)
    (bind _asstatic_mesh_component (Utilities|Casting|CastToStaticMeshComponent InteractTarget))
    (if (== _asstatic_mesh_component (Variables|Default|GetCupboard))
      (Variables|Default|SetbCanOpen true :!label _label)
      (else
        (CallFunction|DrawerFlipFlop _asstatic_mesh_component)
        (bind _open_drawer (Timeline|Timeline PlayFromStart)
          (:Update
            (Transformation|SetRelativeLocation (Variables|Components|GetSM_REF) (Math|Vector|Lerp(Vector) (Variables|Default|GetStartLocation) (Variables|Default|GetEndLocation) _open_drawer) false false))
          (:Finished
            (goto _label)))))))

(event EventShowPromptSET
  (params (bIsShow :type Boolean))
  ;[0.05098 0.05098 0.05098] Widget_IO_according to the player is in the Trigger Area or not
  (if bIsShow
    (if (not (Variables|Default|GetbWidgetIsExist))
      (bind _returnvalue (UserInterface|CreateWidget "/Game/Developers/LinYanChen/WBP_InteractPrompt.WBP_InteractPrompt_C"))
      (UserInterface|Viewport|AddtoViewport _returnvalue 0)
      (Variables|Default|SetbWidgetIsExist true))
    (else
      (Widget|RemovefromParent _returnvalue)
      (Variables|Default|SetbWidgetIsExist false))))

(fn ConstructionScript
  (|CallParentFunction))