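; BP_Studio is an item inspection studio that shows an item's mesh through a scene capture, with projector and zoom-limit resets.
; Setup copies the InspectItem's mesh and offset transform onto ItemToFocus and enables Tick on demand, though Tick currently does nothing.
; Input switches between the studio and either the regular or tutorial first-person character, detected at BeginPlay.
; A helper swaps glass materials, while bottle-liquid wave code is left unconnected.
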(event EventBeginPlay
  (bind _returnvalue (Game|GetPlayerCharacter 0))
  (bind _asbp_first_person_character (Utilities|Casting|CastToBP_FirstPersonCharacter _returnvalue)
    (:then
      (Variables|Default|SetFirst%20Person _asbp_first_person_character)
      (Variables|Default|SetbIsRegularStage true))
    (:CastFailed
      (bind _asbp_first_person_character_tutorial (Utilities|Casting|CastToBP_FirstPersonCharacterTutorial _returnvalue))
      (Variables|Default|SetFirst%20Person%20Tutorial _asbp_first_person_character_tutorial)
      (Variables|Default|SetbIsRegularStage false))))

(event EventTick
  (params (DeltaSeconds :type Float%20%28single-precision%29))
  (if (Variables|Default|GetbNeedTick)
    _))

(fn ConstructionScript)

(fn AssignItemData
  (params (InspectItem :type BP%20Core%20ITEM%20Object%20Reference) (bIsGlass :type Boolean) (bGlassIsUnite :type Boolean) (GlassDiamondMats :type Array%20of%20Material%20Instance%20Dynamic%20Object%20References) (TotemMat :type Material%20Interface%20Object%20Reference)))

(fn GlassMatUpdate
  (params (bGlassIsUnite :type Boolean) (DiamondMats :type Array%20of%20Material%20Instance%20Dynamic%20Object%20References) (TotemMats :type Material%20Interface%20Object%20Reference))
  (if bGlassIsUnite
    (for (_array_element _array_index) DiamondMats
      (Rendering|Material|SetMaterial (Variables|Default|GetItemToFocus) (+ _array_index 4) _array_element)
      (Rendering|Material|SetMaterial (Variables|Default|GetItemToFocus) 3 TotemMats))
    (else
      (Rendering|Material|SetMaterial (Variables|Default|GetItemToFocus) 3 TotemMats))))

(fn InitProjector
  (Transformation|SetRelativeLocation (Variables|Default|GetSceneCapture) "-70.000000,0.000000,0.000000" false false)
  (Variables|Default|SetbReachZoomCeiling false)
  (Variables|Default|SetbReachZoomFloor false))

(fn ItemTickReset
  (bind _output_get (Variables|Default|SetbNeedTick false))
  (Actor|Tick|SetActorTickEnabled _output_get))

(fn ItemTickSetup
  (params (bNeedTick :type Boolean) (OBJSerialCode :type Name))
  (bind _output_get (Variables|Default|SetbNeedTick bNeedTick))
  (if _output_get
    (Actor|Tick|SetActorTickEnabled true)))

(fn SetupInspectorData
  (bind _inspectitem (Variables|Default|GetInspectItem))
  (Utilities|FlowControl|Sequence
    (:then_0
      (Components|StaticMesh|SetStaticMesh (Variables|Default|GetItemToFocus) (Variables|/Script/Engine.StaticMeshComponent|GetStaticMesh (Variables|/Game/Project/Core/InteractOBJ/BP_CoreOBJ.BP_CoreOBJ_C|GetStaticMesh (Variables|Default|GetInspectItem)))))
    (:then_1
      (Transformation|SetRelativeTransform (Variables|Default|GetItemToFocus) (Variables|/Game/Project/Core/InteractOBJ/BP_CoreITEM.BP_CoreITEM_C|GetInspectorInitOffset (Variables|Default|GetInspectItem)) false false))
    (:then_2
      (CallFunction|ItemTickSetup (Variables|/Game/Project/Core/InteractOBJ/BP_CoreITEM.BP_CoreITEM_C|GetbTickWhenInspect _inspectitem) (Variables|/Game/Project/Core/InteractOBJ/BP_CoreOBJ.BP_CoreOBJ_C|GetOBJSerialCode _inspectitem)))))

(fn SwitchInputMode
  (params (bEnterInspectMode :type Boolean))
  (bind _returnvalue (Game|GetPlayerController 0))
  (bind _returnvalue_2 (Game|GetPlayerController 0))
  (LocalVariables|SetL_EnterInspectMode bEnterInspectMode)
  (if (Variables|Default|GetbIsRegularStage)
    (LocalVariables|SetL_TargetPlayer (Variables|Default|GetFirst%20Person))
    (else
      (LocalVariables|SetL_TargetPlayer (Variables|Default|GetFirst%20Person%20Tutorial))))
  (if (LocalVariables|GetL_EnterInspectMode)
    (Input|DisableInput (LocalVariables|GetL_TargetPlayer) _returnvalue_2)
    (Input|EnableInput _returnvalue_2)
    (else
      (Input|DisableInput _returnvalue)
      (Input|EnableInput (LocalVariables|GetL_TargetPlayer) _returnvalue))))