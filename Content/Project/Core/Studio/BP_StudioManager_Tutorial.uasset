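; Tutorial manager for the item preview studios and item inventory, linking both to the tutorial HUD.
; On BeginPlay it spawns Inspect, ItemCollection and drag (DD) studio actors far from the world origin, then binds to the HUD.
; Call events pass items to each studio, with inspect and collection also updating HUD text.
; Items are stored in the first empty array slot, shown in five-slot pages with a wrapping focus index.
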(event Custom|CallStudio_Inspect
  (params (InspectTarget :type BP%20Core%20ITEM%20Object%20Reference))
  ;[0.2575 0.3087 1] Call Studio
  (bind _output_get (Variables|Default|SetREF_InspectITEM InspectTarget))
  (Default|AssignItemData (Variables|Default|GetREF_Studio) _output_get false false (Variables|GLASSDiamond|GetDiamondGroups) (Variables|Default|GetTotemMats))
  (bind _ref_inspectitem (Variables|Default|GetREF_InspectITEM)
    (:then
      (Default|UpdateInspectorTextInfo (Variables|Default|GetREF_CoreHUDTutorial) (Variables|/Game/Project/Core/InteractOBJ/BP_CoreOBJ.BP_CoreOBJ_C|GetOBJSerialCode _ref_inspectitem))
      (Variables|/Script/Engine.PlayerController|SetbShowMouseCursor (Game|GetPlayerController 0) true))
    (:else
      (Default|UpdateInspectorTextInfo (Variables|Default|GetREF_CoreHUDTutorial) "None99999"))))

(event Custom|CloseStudio
  ;[0.2575 0.3087 1] Call Studio
  (Rendering|SetActorHiddenInGame (Variables|Default|GetREF_Studio) false))

(event Custom|CallHUD_CloseCollection
  ;[0.2575 0.3087 1] Begin / Bind Events
  (Default|CloseItemCollection (Variables|Default|GetREF_CoreHUDTutorial))
  (Variables|Default|SetbIsListMode true))

(event Custom|CallStudio_ItemCollection
  (params (InspectTarget :type BP%20Core%20ITEM%20Object%20Reference))
  ;[0.2575 0.3087 1] Call Studio
  (bind _output_get (Variables|Default|SetREF_InspectITEM InspectTarget))
  (Default|AssignItemData (Variables|Default|GetREF_Studio_E) _output_get false false (Variables|GLASSDiamond|GetDiamondGroups) (Variables|Default|GetTotemMats))
  (bind _ref_inspectitem (Variables|Default|GetREF_InspectITEM)
    (:then
      (Default|UpdateCollectionTextInfo (Variables|Default|GetREF_CoreHUDTutorial) (Variables|/Game/Project/Core/InteractOBJ/BP_CoreOBJ.BP_CoreOBJ_C|GetOBJSerialCode _ref_inspectitem))
      (Variables|/Script/Engine.PlayerController|SetbShowMouseCursor (Game|GetPlayerController 0) true))
    (:else
      (Default|UpdateCollectionTextInfo (Variables|Default|GetREF_CoreHUDTutorial) "None99999"))))

(event Custom|Collection%20Activate
  ;[0.2575 0.3087 1] Begin / Bind Events
  (Variables|Default|SetbIsListMode false)
  (Variables|Default|SetFocusIndex 0)
  (CallFunction|RefreshStudioandFocusFrame))

(event Custom|CallStudio_ItemDrag
  (params (SlotCode :type Integer))
  ;[0.2575 0.3087 1] Call Studio
  (bind _output_get (Variables|Default|SetOnDragCode SlotCode))
  (Default|AssignItemData (Variables|Default|GetREF_Studio_DD) (Utilities|Struct|BreakST_ItemCollection (Utilities|Array|Get(acopy) (Variables|Default|GetData_ITEM) _output_get)) false false (Variables|GLASSDiamond|GetDiamondGroups) (Variables|Default|GetTotemMats))
  (Default|SwitchDDState (Variables|Default|GetREF_Studio_DD) true))

(event Custom|BindAllEvents
  ;[0.2575 0.3087 1] Begin / Bind Events
  (EventDispatchers|BindEventtoCloseCollection (Variables|Default|GetREF_Studio_E) (delegate Custom|CallHUD_CloseCollection)))

(event EventBeginPlay
  ;[0.2575 0.3087 1] Begin / Bind Events
  (CallFunction|SpawnStudios)
  (bind _asbp_core_hudtutorial (Utilities|GetCoreHUDinTimeTutorial 1e+01)
    (:Success
      (Variables|Default|SetREF_CoreHUDTutorial _asbp_core_hudtutorial)
      (Utilities|FlowControl|DelayUntilNextTick)
      (CallFunction|BindAllEvents)
      (Default|AssignDDtoDragUIs (Variables|Default|GetREF_CoreHUDTutorial) (Variables|Default|GetREF_Studio_DD)))))

(fn ConstructionScript)

(fn CheckFirstEmptyElem
  (bind (_array_element _array_index) (Utilities|Array|ForEachLoopwithBreak (Variables|Default|GetData_ITEM) :!label _label)
    (:LoopBody
      (if (== (Utilities|Struct|BreakST_ItemCollection _array_element) -1)
        (Variables|Default|SetFirstEmptyElem_ITEM _array_index)
        (goto _label Break)))))

(fn CheckFocusFrameIndex
  (params (bMoveUp :type Boolean))
  (if bMoveUp
    (LocalVariables|SetL_MoveCount -1)
    (else
      (LocalVariables|SetL_MoveCount 1)))
  (Utilities|FlowControl|Sequence
    (:then_0
      (Variables|Default|SetFocusIndex (+ (Variables|Default|GetFocusIndex) (LocalVariables|GetL_MoveCount))))
    (:then_1
      (if (> (Variables|Default|GetFocusIndex) 4)
        (Variables|Default|SetFocusIndex 0)
        (elif (< (Variables|Default|GetFocusIndex) 0)
          (Variables|Default|SetFocusIndex 4))))))

(fn ClearITEMdata
  (Utilities|Array|SetArrayElem :TargetArray (Variables|Default|GetData_ITEM) :Index (Variables|Default|GetOnDragCode))
  (if (< (Variables|Default|GetOnDragCode) (Variables|Default|GetFirstEmptyElem_ITEM))
    (Variables|Default|SetFirstEmptyElem_ITEM (Variables|Default|GetOnDragCode)))
  (Default|ClearSingleITEMData (Variables|Default|GetREF_CoreHUDTutorial) (- (Variables|Default|GetOnDragCode) (* (Variables|Default|GetCurrentPage_ITEM) 5)))
  (Variables|Default|SetOnDragCode -1)
  (Math|Integer|DecrementInt (Variables|Default|GetTotal_ITEM)))

(fn GetCurrentProjectData
  (return (Utilities|Struct|BreakST_ItemCollection (Utilities|Array|Get(acopy) (Variables|Default|GetData_ITEM) (+ (Variables|Default|GetFocusIndex) (* (Variables|Default|GetCurrentPage_ITEM) 5))))))

(fn RefreshStudioandFocusFrame
  (bind _currentpage_item (Variables|Default|GetCurrentPage_ITEM))
  (bind _data_item (Variables|Default|GetData_ITEM))
  (bind _returnvalue (* _currentpage_item 5))
  (bind _output (Utilities|Array|Get(acopy) _data_item _returnvalue))
  (bind _targetitemactor (Utilities|Struct|BreakST_ItemCollection _output))
  (CallFunction|CallStudioItemCollection _targetitemactor)
  (Default|RequestMoveFocusFrame (Variables|Default|GetREF_CoreHUDTutorial) (Variables|Default|GetFocusIndex) (Utilities|IsValid _targetitemactor)))

(fn SpawnStudios
  (Utilities|FlowControl|Sequence
    (:then_0
      (bind _returnvalue (Game|SpawnActorfromClass "/Game/Project/Core/Studio/BP_Studio_Inspect.BP_Studio_Inspect_C" (Math|Transform|MakeTransform "1000000000.000000,0.000000,0.000000") "Undefined" 0 0))
      (Variables|Default|SetREF_Studio _returnvalue))
    (:then_1
      (bind _returnvalue_2 (Game|SpawnActorfromClass "/Game/Project/Core/Studio/BP_Studio_ItemCollection.BP_Studio_ItemCollection_C" (Math|Transform|MakeTransform "1000000000.000000,0.000000,1000000000.000000") "Undefined" 0 0))
      (Variables|Default|SetREF_Studio_E _returnvalue_2))
    (:then_2
      (bind _returnvalue_3 (Game|SpawnActorfromClass "/Game/Project/Core/Studio/BP_Studio_DD.BP_Studio_DD_C" (Math|Transform|MakeTransform "1000000000.000000,0.000000,2000000000.000000") "Undefined" 0 0))
      (Variables|Default|SetREF_Studio_DD _returnvalue_3))))

(fn StoreITEMData
  (params (TargetITEM :type BP%20Core%20ITEM%20Object%20Reference))
  (bind _firstemptyelem_item (Variables|Default|GetFirstEmptyElem_ITEM))
  (bind _firstemptyelem_item_2 (Variables|Default|GetFirstEmptyElem_ITEM))
  (bind _currentpage_item (Variables|Default|GetCurrentPage_ITEM))
  (bind _firstemptyelem_item_3 (Variables|Default|GetFirstEmptyElem_ITEM))
  (bind _returnvalue (* _currentpage_item 5))
  (bind _output_get (LocalVariables|SetL_TargetITEM TargetITEM))
  (bind _extractdata (Class|BICoreOBJInspectInterface|GetExtractData(Message) _output_get))
  (Utilities|Array|SetArrayElem (Variables|Default|GetData_ITEM) _firstemptyelem_item (Utilities|Struct|MakeST_ItemCollection (LocalVariables|GetL_TargetITEM) _firstemptyelem_item (Variables|/Game/Project/Core/InteractOBJ/BP_CoreITEM.BP_CoreITEM_C|GetItemPreview (LocalVariables|GetL_TargetITEM)) (Variables|/Game/Project/Core/InteractOBJ/BP_CoreITEM.BP_CoreITEM_C|GetInspectorInitOffset (LocalVariables|GetL_TargetITEM)) (Variables|/Game/Project/Core/InteractOBJ/BP_CoreOBJ.BP_CoreOBJ_C|GetThisOBJtype (LocalVariables|GetL_TargetITEM)) _extractdata (Variables|/Game/Project/Core/InteractOBJ/BP_CoreITEM.BP_CoreITEM_C|GetInteractSE (LocalVariables|GetL_TargetITEM))))
  (if (and (>= _firstemptyelem_item_3 _returnvalue) (<= _firstemptyelem_item_3 (+ _returnvalue 4)))
    (Default|AssignSingleITEMData (Variables|Default|GetREF_CoreHUDTutorial) (Utilities|Array|Get(acopy) (Variables|Default|GetData_ITEM) _firstemptyelem_item_2) (- _firstemptyelem_item_2 (* (Variables|Default|GetCurrentPage_ITEM) 5))))
  (CallFunction|CheckFirstEmptyElem)
  (Math|Integer|IncrementInt (Variables|Default|GetTotal_ITEM)))