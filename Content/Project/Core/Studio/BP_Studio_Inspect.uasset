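; Studio Blueprint for inspecting items, showing the assigned item to a scene capture alongside the first-person or tutorial inspector UI.
; AssignItemData loads the item's offset and zoom step, updates glass materials, switches input mode, then floats the item up on a timeline.
; Left-drag rotates the item, the wheel moves the capture within zoom limits, and right-click or the inspector action floats it out.
; Setup, input-mode and material functions defer to the parent class.
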(event Custom|InspectorShowup
  (bind _initlocation (Variables|Default|GetInitLocation))
  ;[0.2575 0.3087 1] Begin / Tick / Activate
  (Components|Activation|Activate (Variables|Default|GetSceneCapture) false)
  (bind _showingtrack (Timeline|ItemFloatIn PlayFromStart)
    (:Update
      (Transformation|SetRelativeLocation (Variables|Default|GetItemToFocus) (Math|Vector|Lerp(Vector) (Math|Vector|MakeVector (.x _initlocation) (.y _initlocation) -1e+02) (Variables|Default|GetInitLocation) _showingtrack) false false))))

(event Input|EnhancedActionEvents|EnhancedInputActionIA_ItemCollectionInspector
  (params (ActionValue :type Boolean) (ElapsedSeconds :type Float%20%28double-precision%29) (TriggeredSeconds :type Float%20%28double-precision%29) (InputAction :type Input%20Action%20Object%20Reference :default "/Game/ProjectDefault/FirstPerson/Input/Actions/IA_ItemCollectionInspector.IA_ItemCollectionInspector"))
  (bind _first_person (Variables|Default|GetFirst%20Person))
  (bind _first_person_tutorial (Variables|Default|GetFirst%20Person%20Tutorial))
  (bind _initlocation (Variables|Default|GetInitLocation))
  ;[0.2575 0.3087 1] Exit
  (:Triggered
    (CallFunction|SwitchInputMode false)
    (bind _showingtrack (Timeline|ItemFloatOut ReverseFromEnd)
      (:Update
        (Transformation|SetRelativeLocation (Variables|Default|GetItemToFocus) (Math|Vector|Lerp(Vector) (Math|Vector|MakeVector (.x _initlocation) (.y _initlocation) -1e+02) (Variables|Default|GetInitLocation) _showingtrack) false false))
      (:Finished
        (if (Variables|Default|GetbIsRegularStage)
          (Default|CallInspectorUI _first_person false)
          (Default|ITEMDetach _first_person)
          (CallFunction|ItemTickReset)
          (else
            (Default|CallInspectorUI _first_person_tutorial false)
            (Default|ITEMDetach _first_person_tutorial)))
        (Components|Activation|Deactivate (Variables|Default|GetSceneCapture))))))

(event EventBeginPlay
  ;[0.2575 0.3087 1] Begin / Tick / Activate
  (|CallParentFunction)
  (Components|Activation|Deactivate (Variables|Default|GetSceneCapture)))

(event EventTick
  (params (DeltaSeconds :type Float%20%28single-precision%29))
  ;[0.2575 0.3087 1] Begin / Tick / Activate
)

(event Input|MouseEvents|MouseX
  (params (AxisValue :type Float%20%28single-precision%29))
  ;[0.2575 0.3087 1] Rotate
  (if (Variables|Default|GetbIsRotating)
    (Transformation|SetWorldRotation (Variables|Default|GetItemToFocus) (Math|Rotator|CombineRotators (Transformation|GetWorldRotation (Variables|Default|GetItemToFocus)) (Math|Rotator|MakeRotator 0.0 0.0 (* AxisValue -2.0))) false false)))

(event Input|MouseEvents|MouseY
  (params (AxisValue :type Float%20%28single-precision%29))
  ;[0.2575 0.3087 1] Rotate
  (if (Variables|Default|GetbIsRotating)
    (Transformation|SetWorldRotation (Variables|Default|GetItemToFocus) (Math|Rotator|CombineRotators (Transformation|GetWorldRotation (Variables|Default|GetItemToFocus)) (Math|Rotator|MakeRotator 0.0 (* AxisValue -2.0) 0.0)) false false)))

(event Input|MouseEvents|RightMouseButton
  (params (Key :type Key%20Structure :default "None"))
  (bind _first_person (Variables|Default|GetFirst%20Person))
  (bind _first_person_tutorial (Variables|Default|GetFirst%20Person%20Tutorial))
  (bind _initlocation (Variables|Default|GetInitLocation))
  ;[0.2575 0.3087 1] Exit
  (:Pressed
    (CallFunction|SwitchInputMode false)
    (bind _showingtrack (Timeline|ItemFloatOut ReverseFromEnd)
      (:Update
        (Transformation|SetRelativeLocation (Variables|Default|GetItemToFocus) (Math|Vector|Lerp(Vector) (Math|Vector|MakeVector (.x _initlocation) (.y _initlocation) -1e+02) (Variables|Default|GetInitLocation) _showingtrack) false false))
      (:Finished
        (if (Variables|Default|GetbIsRegularStage)
          (Default|CallInspectorUI _first_person false)
          (Default|ITEMDetach _first_person)
          (CallFunction|ItemTickReset)
          (else
            (Default|CallInspectorUI _first_person_tutorial false)
            (Default|ITEMDetach _first_person_tutorial)))
        (Components|Activation|Deactivate (Variables|Default|GetSceneCapture))))))

(event Input|MouseEvents|LeftMouseButton
  (params (Key :type Key%20Structure :default "None"))
  ;[0.2575 0.3087 1] Rotate
  (:Pressed
    (Variables|Default|SetbIsRotating true))
  (:Released
    (Variables|Default|SetbIsRotating false)))

(event Input|MouseEvents|MouseWheelUp
  (params (Key :type Key%20Structure :default "None"))
  (bind _scenecapture (Variables|Default|GetSceneCapture))
  (bind _relativelocation (Variables|/Script/Engine.SceneComponent|GetRelativeLocation _scenecapture))
  ;[0.2575 0.3087 1] Scaling
  (:Pressed
    (Variables|Default|SetbReachZoomFloor false)
    (if (not (Variables|Default|GetbReachZoomCeiling))
      (Transformation|SetRelativeLocation (Variables|Default|GetSceneCapture) (Math|Vector|MakeVector (+ (Variables|Default|GetScale%20Units) (.x _relativelocation)) (.y _relativelocation) (.z _relativelocation)) false false)
      (if (>= (.x (Variables|/Script/Engine.SceneComponent|GetRelativeLocation (Variables|Default|GetSceneCapture))) (+ -7e+01 (* (Variables|Default|GetScale%20Units) 1e+01)))
        (Variables|Default|SetbReachZoomCeiling true)))))

(event Input|MouseEvents|MouseWheelDown
  (params (Key :type Key%20Structure :default "None"))
  (bind _scenecapture (Variables|Default|GetSceneCapture))
  (bind _relativelocation (Variables|/Script/Engine.SceneComponent|GetRelativeLocation _scenecapture))
  ;[0.2575 0.3087 1] Scaling
  (:Pressed
    (Variables|Default|SetbReachZoomCeiling false)
    (if (not (Variables|Default|GetbReachZoomFloor))
      (Transformation|SetRelativeLocation (Variables|Default|GetSceneCapture) (Math|Vector|MakeVector (- (.x _relativelocation) (Variables|Default|GetScale%20Units)) (.y _relativelocation) (.z _relativelocation)) false false)
      (if (<= (.x (Variables|/Script/Engine.SceneComponent|GetRelativeLocation (Variables|Default|GetSceneCapture))) (+ -7e+01 (* (Variables|Default|GetScale%20Units) -1e+01)))
        (Variables|Default|SetbReachZoomFloor true)))))

(fn ConstructionScript)

(fn AssignItemData
  (params (InspectItem :type BP%20Core%20ITEM%20Object%20Reference) (bIsGlass :type Boolean) (bGlassIsUnite :type Boolean) (GlassDiamondMats :type Array%20of%20Material%20Instance%20Dynamic%20Object%20References) (TotemMat :type Material%20Interface%20Object%20Reference))
  (Variables|Default|SetInspectItem InspectItem)
  (Utilities|FlowControl|Sequence
    (:then_0
      (Variables|Default|SetInitLocation (.location (Variables|/Game/Project/Core/InteractOBJ/BP_CoreITEM.BP_CoreITEM_C|GetInspectorInitOffset InspectItem)))
      (Variables|Default|SetScale%20Units (Variables|/Game/Project/Core/InteractOBJ/BP_CoreITEM.BP_CoreITEM_C|GetScaleUnits InspectItem)))
    (:then_1
      (if bIsGlass
        (CallFunction|GlassMatUpdate bGlassIsUnite GlassDiamondMats TotemMat))
      (if (Variables|Default|GetbIsRegularStage)
        (Default|CallInspectorUI (Variables|Default|GetFirst%20Person) true)
        (else
          (Default|CallInspectorUI (Variables|Default|GetFirst%20Person%20Tutorial) true)))
      (CallFunction|SwitchInputMode true)
      (CallFunction|SetupInspectorData)
      (CallFunction|InitProjector)
      (CallFunction|InspectorShowup)
      (return))))

(fn GlassMatUpdate
  (params (bGlassIsUnite :type Boolean) (DiamondMats :type Array%20of%20Material%20Instance%20Dynamic%20Object%20References) (TotemMats :type Material%20Interface%20Object%20Reference))
  (|CallParentFunction bGlassIsUnite DiamondMats TotemMats)
  (return))

(fn InitProjector
  (|CallParentFunction))

(fn ItemTickReset
  (|CallParentFunction))

(fn ItemTickSetup
  (params (bNeedTick :type Boolean) (OBJSerialCode :type Name :default "None"))
  (|CallParentFunction bNeedTick OBJSerialCode))

(fn SetupInspectorData
  (|CallParentFunction))

(fn SwitchInputMode
  (params (bEnterInspectMode :type Boolean))
  (|CallParentFunction bEnterInspectMode))