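; BP_Studio_DD is a studio actor that stages an inspected item in front of a scene capture.
; AssignItemData copies the item's mesh and initial inspector rotation and scale onto ItemToFocus.
; For glass items, it also passes unite state, diamond and totem materials to GlassMatUpdate.
; The scene capture is deactivated on BeginPlay and toggled by SwitchDDState, so it is active only on demand.
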(event Custom|SwitchDDState
  (params (bIsActivate :type Boolean))
  (if bIsActivate
    (Components|Activation|Activate (Variables|Default|GetSceneCapture) false)
    (else
      (Components|Activation|Deactivate (Variables|Default|GetSceneCapture)))))

(event EventBeginPlay
  (Components|Activation|Deactivate (Variables|Default|GetSceneCapture)))

(fn ConstructionScript)

(fn SetupInspectorData
  (Components|StaticMesh|SetStaticMesh (Variables|Default|GetItemToFocus) (Variables|/Script/Engine.StaticMeshComponent|GetStaticMesh (Variables|/Game/Project/Core/InteractOBJ/BP_CoreOBJ.BP_CoreOBJ_C|GetStaticMesh (Variables|Default|GetInspectItem))))
  (Transformation|SetRelativeRotation (Variables|Default|GetItemToFocus) (Variables|Default|GetInit%20Rotation) false false)
  (Transformation|SetRelativeScale3D (Variables|Default|GetItemToFocus) (Variables|Default|GetInit%20Scale)))

(fn AssignItemData
  (params (InspectItem :type BP%20Core%20ITEM%20Object%20Reference) (bIsGlass :type Boolean) (bGlassIsUnite :type Boolean) (GlassDiamondMats :type Array%20of%20Material%20Instance%20Dynamic%20Object%20References) (TotemMat :type Material%20Interface%20Object%20Reference))
  (bind _output_get (Variables|Default|SetInspectItem InspectItem))
  (Variables|Default|SetInit%20Rotation (.rotation (Variables|/Game/Project/Core/InteractOBJ/BP_CoreITEM.BP_CoreITEM_C|GetInspectorInitOffset _output_get)))
  (Variables|Default|SetInit%20Scale (.scale (Variables|/Game/Project/Core/InteractOBJ/BP_CoreITEM.BP_CoreITEM_C|GetInspectorInitOffset _output_get)))
  (if bIsGlass
    (CallFunction|GlassMatUpdate bGlassIsUnite GlassDiamondMats TotemMat))
  (CallFunction|SetupInspectorData)
  (return))