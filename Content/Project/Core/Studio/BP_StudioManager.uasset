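; Manager for item preview studios, spawning separate far-off studio actors for inspection, item collection and drag previews.
; Call events extract the target's glass state and totem material, then pass them to the matching studio's AssignItemData.
; UNITE glass lights up to three shared dynamic diamond materials according to its inherit layer.
; Glass drags first refresh the totem render-target material through the glass manager.
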(event Custom|CallStudio
  (params (InspectTarget :type BP%20Core%20ITEM%20Object%20Reference))
  ;[1 1 1] Call Studio Item - Inspect Item
  (bind _output_get (Variables|Default|SetInspectITEM InspectTarget))
  (CallFunction|AssignTargetData _output_get)
  (Default|AssignItemData (Variables|Default|GetREF_Studio) (Variables|Default|GetInspectITEM) (Variables|Default|GetbIsGlass) (Variables|Default|GetbGlassIsUnite) (Variables|Default|GetDiamondGroups) (Variables|Default|GetTotemMats)))

(event Custom|CloseStudio
  ;[1 1 1] Call Studio Item - Inspect Item
  (Rendering|SetActorHiddenInGame (Variables|Default|GetREF_Studio) false))

(event Custom|CallStudio_ItemCollection
  (params (InspectTarget :type BP%20Core%20ITEM%20Object%20Reference))
  ;[1 1 1] Call Studio Item - Item List
  (bind _output_get (Variables|Default|SetInspectITEM InspectTarget))
  (CallFunction|AssignTargetData _output_get)
  (Default|AssignItemData (Variables|Default|GetREF_Studio_E) (Variables|Default|GetInspectITEM) (Variables|Default|GetbIsGlass) (Variables|Default|GetbGlassIsUnite) (Variables|Default|GetDiamondGroups) (Variables|Default|GetTotemMats)))

(event Custom|CloseStudio_ItemCollection
  ;[1 1 1] Call Studio Item - Item List
  (Rendering|SetActorHiddenInGame (Variables|Default|GetREF_Studio_E) false))

(event Custom|CallStudio_ItemCollection_ButEmpty
  ;[1 1 1] Call Studio Item - Item List
  (Default|AssignItemData (Variables|Default|GetREF_Studio_E) 0 (Variables|Default|GetbIsGlass) (Variables|Default|GetbGlassIsUnite) (Variables|Default|GetDiamondGroups) (Variables|Default|GetTotemMats)))

(event Custom|CallStudio_GlassBaseDrag
  (params (GlassType :type E_GLASSType%20Enum :default "NewEnumerator6") (Target%20Valid%20Data%20Base :type ST%20Glass%20Data%20Structure) (Target%20Valid%20Data%20Unite :type ST%20Glass%20Data%20Structure))
  ;[1 1 1] Call Studio Item - Drag Item
  (switch Utilities|FlowControl|Switch|SwitchonE_GLASSType GlassType
    (:NewEnumerator6
      (Variables|Default|SetInspectITEM (Utilities|Struct|BreakST_GlassData Target%20Valid%20Data%20Base)))
    (:NewEnumerator1
      (Variables|Default|SetInspectITEM (Utilities|Struct|BreakST_GlassData Target%20Valid%20Data%20Unite))))
  (CallFunction|AssignTargetDataCache 0 (Variables|Default|GetInspectITEM))
  (Default|AssignItemData (Variables|Default|GetREF_Studio_DD) (Variables|Default|GetInspectITEM) (Variables|Default|GetbIsGlass) (Variables|Default|GetbGlassIsUnite) (Variables|Default|GetDiamondGroups) (Variables|Default|GetTotemMats)))

(event Custom|CallStudio_GlassCollection
  (params (InspectGlass :type BP%20Core%20ITEM%20GLASS%20Object%20Reference))
  (bind _output_get (Variables|Default|SetInspectITEM InspectGlass))
  (CallFunction|AssignTargetData _output_get)
  (Default|AssignItemData (Variables|Default|GetREF_Studio_E) (Variables|Default|GetInspectITEM) (Variables|Default|GetbIsGlass) (Variables|Default|GetbGlassIsUnite) (Variables|Default|GetDiamondGroups) (Variables|Default|GetTotemMats)))

(event Custom|CallStudio_ItemDrag
  (params (Target%20Valid%20Data :type ST%20Item%20Collection%20Structure))
  ;[1 1 1] Call Studio Item - Drag Item
  (bind _asbp_core_item (Utilities|Casting|CastToBP_CoreITEM (Utilities|Struct|BreakST_ItemCollection Target%20Valid%20Data)))
  (bind _output_get (Variables|Default|SetInspectITEM _asbp_core_item))
  (CallFunction|AssignTargetData _output_get)
  (Default|AssignItemData (Variables|Default|GetREF_Studio_DD) (Variables|Default|GetInspectITEM) (Variables|Default|GetbIsGlass) (Variables|Default|GetbGlassIsUnite) (Variables|Default|GetDiamondGroups) (Variables|Default|GetTotemMats)))

(event EventBeginPlay
  (CallFunction|SpawnStudios))

(fn ConstructionScript
  (CallFunction|CreateDiamondMat))

(fn AssignTargetData
  (params (TargetInspect :type BP%20Core%20ITEM%20Object%20Reference))
  (LocalVariables|SetL_TargetInspect 0)
  (bind _asbp_glassitem (Utilities|Casting|CastToBP_GLASSItem TargetInspect)
    (:then
      (Variables|Default|SetbIsGlass true)
      (Variables|Default|SetTotemMats (Rendering|Material|GetMaterial (Variables|/Game/Project/Core/InteractOBJ/BP_CoreOBJ.BP_CoreOBJ_C|GetStaticMesh _asbp_glassitem) 3))
      (bind _output_get (Variables|Default|SetbGlassIsUnite (Utilities|Enum|Equal(Enum) (Variables|/Game/Project/Core/InteractOBJ/BP_CoreITEM_GLASS.BP_CoreITEM_GLASS_C|GetGlassType _asbp_glassitem) "NewEnumerator1")))
      (if _output_get
        (CallFunction|SetInheritDiamond _asbp_glassitem)))
    (:CastFailed
      (Variables|Default|SetbIsGlass false)
      (Variables|Default|SetbGlassIsUnite false)))
  (return))

(fn AssignTargetDataCache
  (params (TargetInspectOld :type BP%20Core%20OBJ%20Object%20Reference) (TargetInspect :type BP%20Core%20ITEM%20Object%20Reference))
  (LocalVariables|SetL_TargetInspect_Old TargetInspectOld)
  (LocalVariables|SetL_TargetInspect TargetInspect)
  (Variables|Default|SetbIsGlass false)
  (Variables|Default|SetbGlassIsUnite false)
  (bind _asbp_glassitem (Utilities|Casting|CastToBP_GLASSItem (LocalVariables|GetL_TargetInspect))
    (:then
      (LocalVariables|SetL_TargetGlassItem _asbp_glassitem)
      (Utilities|FlowControl|Sequence
        (:then_0
          (Variables|Default|SetbIsGlass true)
          (Default|UpdateTotemRTScene (Variables|/Game/Project/InteractOBJ/BP_GLASSItem.BP_GLASSItem_C|GetREF_GlassManager (LocalVariables|GetL_TargetGlassItem)) (.glassvalue (Variables|/Game/Project/InteractOBJ/BP_GLASSItem.BP_GLASSItem_C|GetThisGlass (LocalVariables|GetL_TargetGlassItem))) 5)
          (bind _previewmat (Default|ReturnRenderMatScene (Variables|/Game/Project/InteractOBJ/BP_GLASSItem.BP_GLASSItem_C|GetREF_GlassManager (LocalVariables|GetL_TargetGlassItem)) 5))
          (Rendering|Material|SetMaterial (Variables|/Game/Project/Core/InteractOBJ/BP_CoreOBJ.BP_CoreOBJ_C|GetStaticMesh (LocalVariables|GetL_TargetGlassItem)) 3 _previewmat))
        (:then_1
          (Variables|Default|SetTotemMats (Rendering|Material|GetMaterial (Variables|/Game/Project/Core/InteractOBJ/BP_CoreOBJ.BP_CoreOBJ_C|GetStaticMesh (LocalVariables|GetL_TargetGlassItem)) 3))
          (bind _output_get (Variables|Default|SetbGlassIsUnite (Utilities|Enum|Equal(Enum) (Variables|/Game/Project/Core/InteractOBJ/BP_CoreITEM_GLASS.BP_CoreITEM_GLASS_C|GetGlassType (LocalVariables|GetL_TargetGlassItem)) "NewEnumerator1")))
          (if _output_get
            (CallFunction|SetInheritDiamond (LocalVariables|GetL_TargetGlassItem)))
          (return))))
    (:CastFailed
      (return))))

(fn CreateDiamondMat
  (Utilities|FlowControl|Sequence
    (:then_0
      (bind _returnvalue (Rendering|Material|CreateDynamicMaterialInstance "/Game/Project/Artist/KeyObj/Material/Slider_Diamond00.Slider_Diamond00" "None" "None" :!class /Script/Engine.KismetMaterialLibrary))
      (bind _output_get (Variables|Default|SetDiamond_L _returnvalue))
      (Utilities|Array|Add (Variables|Default|GetDiamondGroups) _output_get))
    (:then_1
      (bind _returnvalue_2 (Rendering|Material|CreateDynamicMaterialInstance "/Game/Project/Artist/KeyObj/Material/Slider_Diamond02.Slider_Diamond02" "None" "None" :!class /Script/Engine.KismetMaterialLibrary))
      (bind _output_get_2 (Variables|Default|SetDiamond_R _returnvalue_2))
      (Utilities|Array|Add (Variables|Default|GetDiamondGroups) _output_get_2))
    (:then_2
      (bind _returnvalue_3 (Rendering|Material|CreateDynamicMaterialInstance "/Game/Project/Artist/KeyObj/Material/Slider_Diamond01.Slider_Diamond01" "None" "None" :!class /Script/Engine.KismetMaterialLibrary))
      (bind _output_get_3 (Variables|Default|SetDiamond_M _returnvalue_3))
      (Utilities|Array|Add (Variables|Default|GetDiamondGroups) _output_get_3))
    (:then_3
      (for _array_element (Variables|Default|GetDiamondGroups)
        (Rendering|Material|SetScalarParameterValue _array_element "Enable" 0.0 :!class /Script/Engine.MaterialInstanceDynamic)
        (Rendering|Material|SetScalarParameterValue _array_element "Speed" 0.0 :!class /Script/Engine.MaterialInstanceDynamic)))))

(fn SetInheritDiamond
  (params (UniteGlass :type BP%20GLASS%20Item%20Object%20Reference))
  (LocalVariables|SetL_Layer (.inheritlayer (Variables|/Game/Project/InteractOBJ/BP_GLASSItem.BP_GLASSItem_C|GetThisGlass UniteGlass)))
  (for _index (range 0 2)
    (bind _output_get (LocalVariables|SetL_LoopIndex _index))
    (if (< _output_get (LocalVariables|GetL_Layer))
      (Rendering|Material|SetScalarParameterValue (Utilities|Array|Get(acopy) (Variables|Default|GetDiamondGroups) (LocalVariables|GetL_LoopIndex)) "Enable" 1.0 :!class /Script/Engine.MaterialInstanceDynamic)
      (Rendering|Material|SetScalarParameterValue (Utilities|Array|Get(acopy) (Variables|Default|GetDiamondGroups) (LocalVariables|GetL_LoopIndex)) "Speed" 0.1 :!class /Script/Engine.MaterialInstanceDynamic)
      (else
        (Rendering|Material|SetScalarParameterValue (Utilities|Array|Get(acopy) (Variables|Default|GetDiamondGroups) (LocalVariables|GetL_LoopIndex)) "Enable" 0.0 :!class /Script/Engine.MaterialInstanceDynamic)
        (Rendering|Material|SetScalarParameterValue (Utilities|Array|Get(acopy) (Variables|Default|GetDiamondGroups) (LocalVariables|GetL_LoopIndex)) "Speed" 0.0 :!class /Script/Engine.MaterialInstanceDynamic)))))

(fn SpawnStudios
  (Utilities|FlowControl|Sequence
    (:then_0
      (bind _returnvalue (Game|SpawnActorfromClass "/Game/Project/Core/Studio/BP_Studio_Inspect.BP_Studio_Inspect_C" (Math|Transform|MakeTransform "1000000000.000000,0.000000,0.000000") "Undefined" 0 0))
      (Variables|Default|SetREF_Studio _returnvalue))
    (:then_1
      (bind _returnvalue_2 (Game|SpawnActorfromClass "/Game/Project/Core/Studio/BP_Studio_ItemCollection.BP_Studio_ItemCollection_C" (Math|Transform|MakeTransform "1000000000.000000,0.000000,1000000000.000000") "Undefined" 0 0))
      (Variables|Default|SetREF_Studio_E _returnvalue_2))
    (:then_2
      (bind _returnvalue_3 (Game|SpawnActorfromClass "/Game/Project/Core/Studio/BP_Studio_DD.BP_Studio_DD_C" (Math|Transform|MakeTransform "1000000000.000000,0.000000,2000000000.000000") "Undefined" 0 0))
      (Variables|Default|SetREF_Studio_DD _returnvalue_3))))