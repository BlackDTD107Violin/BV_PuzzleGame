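; Item inspection studio actor that shows a collected item's mesh to a scene capture for the player's inspector UI.
; AssignInspectorData sets mesh, offset and optional glass materials, takes input from the regular or tutorial character, and slides the item up.
; Left-drag rotates, the wheel moves the capture for bounded zoom, and right-click or the inspector action reverses out.
; Certain items enable Tick to drive a liquid material's wave while rotating.
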(event Custom|InteractInspection
  (params (FirstPerson :type BP%20First%20Person%20Character%20Object%20Reference) (FirstPersonTutorial :type BP%20First%20Person%20Character%20Tutorial%20Object%20Reference))
  (bind _returnvalue (Game|GetPlayerController 0))
  (bind _returnvalue_2 (Game|GetPlayerController 0))
  (Utilities|IsValid FirstPerson
    (:Is%20Valid
      (Input|DisableInput _returnvalue_2)
      (Input|EnableInput (Variables|Default|GetFirst%20Person) _returnvalue_2))
    (:Is%20Not%20Valid
      (Utilities|IsValid FirstPersonTutorial
        (:Is%20Valid
          (Input|DisableInput _returnvalue)
          (Input|EnableInput (Variables|Default|GetFirst%20Person%20Tutorial) _returnvalue))))))

(event Input|EnhancedActionEvents|EnhancedInputActionIA_ItemCollectionInspector
  (params (ActionValue :type Boolean) (ElapsedSeconds :type Float%20%28double-precision%29) (TriggeredSeconds :type Float%20%28double-precision%29) (InputAction :type Input%20Action%20Object%20Reference :default "/Game/ProjectDefault/FirstPerson/Input/Actions/IA_ItemCollectionInspector.IA_ItemCollectionInspector"))
  (bind _initlocation (Variables|Default|GetInitLocation))
  (:Triggered
    (CallFunction|SwitchInputMode false)
    (bind _showingtrack (Timeline|Timeline_1 ReverseFromEnd)
      (:Update
        (Transformation|SetRelativeLocation (Variables|Default|GetItemToFocusMain) (Math|Vector|Lerp(Vector) (Math|Vector|MakeVector (.x _initlocation) (.y _initlocation) -1e+02) (Variables|Default|GetInitLocation) _showingtrack) false false))
      (:Finished
        (if (Variables|Default|GetbIsRegularStage)
          (Default|CallInspectorUI (Variables|Default|GetFirst%20Person) false)
          (Default|OBJDetach (Variables|Default|GetFirst%20Person))
          (CallFunction|ItemTickReset)
          (else
            (Default|CallInspectorUI (Variables|Default|GetFirst%20Person%20Tutorial) false)
            (Default|OBJDetach (Variables|Default|GetFirst%20Person%20Tutorial))))))))

(event EventBeginPlay
  (bind _returnvalue (Game|GetPlayerCharacter 0))
  (bind _asbp_first_person_character (Utilities|Casting|CastToBP_FirstPersonCharacter _returnvalue)
    (:then
      (Variables|Default|SetFirst%20Person _asbp_first_person_character)
      (Variables|Default|SetbIsRegularStage true))
    (:CastFailed
      (bind _asbp_first_person_character_tutorial (Utilities|Casting|CastToBP_FirstPersonCharacterTutorial _returnvalue))
      (Variables|Default|SetFirst%20Person%20Tutorial _asbp_first_person_character_tutorial)
      (Variables|Default|SetbIsRegularStage false))))

(event EventTick
  (params (DeltaSeconds :type Float%20%28single-precision%29))
  (if (Variables|Default|GetbNeedTick)
    (if (Variables|Default|GetbIsRotating)
      (Variables|Default|SetLiquidWaveTime 0.2)
      (else
        (Variables|Default|SetLiquidWaveTime 0.05)))
    (Rendering|Material|SetScalarParameterValue (Variables|Default|GetK1002_Liquid) "WaveTime" (Variables|Default|GetLiquidWaveTime) :!class /Script/Engine.MaterialInstanceDynamic)))

(event EventGlassMatModify
  (params (bGlassIsUnite :type Boolean) (DiamondMats :type Array%20of%20Material%20Instance%20Dynamic%20Object%20References) (TotemMats :type Material%20Interface%20Object%20Reference))
  (if bGlassIsUnite
    (for (_array_element _array_index) DiamondMats
      (Rendering|Material|SetMaterial (Variables|Default|GetItemToFocusMain) (+ _array_index 4) _array_element)
      (Rendering|Material|SetMaterial (Variables|Default|GetItemToFocusMain) 3 TotemMats))
    (else
      (Rendering|Material|SetMaterial (Variables|Default|GetItemToFocusMain) 3 TotemMats))))

(event EventAssignInspectorData
  (params (InspectTarget :type BP%20Core%20OBJ%20Object%20Reference) (bIsGlass :type Boolean) (bGlassIsUnite :type Boolean) (GlassDiamondMats :type Array%20of%20Material%20Instance%20Dynamic%20Object%20References) (TotemMat :type Material%20Interface%20Object%20Reference))
  (bind _output_get (Variables|Default|SetInspect%20Target InspectTarget))
  (Variables|Default|SetInitLocation (.location (Variables|/Game/Project/Core/InteractOBJ/BP_CoreOBJ.BP_CoreOBJ_C|GetInspectorInitOffset _output_get)))
  (Variables|Default|SetScale%20Units (Variables|/Game/Project/Core/InteractOBJ/BP_CoreOBJ.BP_CoreOBJ_C|GetScaleUnits _output_get))
  (if bIsGlass
    (CallFunction|GlassMatModify bGlassIsUnite GlassDiamondMats TotemMat))
  (if (Variables|Default|GetbIsRegularStage)
    (Default|CallInspectorUI (Variables|Default|GetFirst%20Person) true)
    (else
      (Default|CallInspectorUI (Variables|Default|GetFirst%20Person%20Tutorial) true)))
  (CallFunction|SwitchInputMode true)
  (CallFunction|SetupInspectorData)
  (CallFunction|InitProjector)
  (bind _showingtrack (Timeline|InspectorShowup PlayFromStart)
    (:Update
      (Transformation|SetRelativeLocation (Variables|Default|GetItemToFocusMain) (Math|Vector|Lerp(Vector) (Math|Vector|MakeVector (.x (Variables|Default|GetInitLocation)) (.y (Variables|Default|GetInitLocation)) -1e+02) (Variables|Default|GetInitLocation) _showingtrack) false false))))

(event Input|MouseEvents|MouseX
  (params (AxisValue :type Float%20%28single-precision%29))
  (if (Variables|Default|GetbIsRotating)
    (Transformation|SetWorldRotation (Variables|Default|GetItemToFocusMain) (Math|Rotator|CombineRotators (Transformation|GetWorldRotation (Variables|Default|GetItemToFocusMain)) (Math|Rotator|MakeRotator 0.0 0.0 (* AxisValue -2.0))) false false)))

(event Input|MouseEvents|MouseY
  (params (AxisValue :type Float%20%28single-precision%29))
  (if (Variables|Default|GetbIsRotating)
    (Transformation|SetWorldRotation (Variables|Default|GetItemToFocusMain) (Math|Rotator|CombineRotators (Transformation|GetWorldRotation (Variables|Default|GetItemToFocusMain)) (Math|Rotator|MakeRotator 0.0 (* AxisValue -2.0) 0.0)) false false)))

(event Input|MouseEvents|RightMouseButton
  (params (Key :type Key%20Structure :default "None"))
  (bind _initlocation (Variables|Default|GetInitLocation))
  (:Pressed
    (CallFunction|SwitchInputMode false)
    (bind _showingtrack (Timeline|Timeline_1 ReverseFromEnd)
      (:Update
        (Transformation|SetRelativeLocation (Variables|Default|GetItemToFocusMain) (Math|Vector|Lerp(Vector) (Math|Vector|MakeVector (.x _initlocation) (.y _initlocation) -1e+02) (Variables|Default|GetInitLocation) _showingtrack) false false))
      (:Finished
        (if (Variables|Default|GetbIsRegularStage)
          (Default|CallInspectorUI (Variables|Default|GetFirst%20Person) false)
          (Default|OBJDetach (Variables|Default|GetFirst%20Person))
          (CallFunction|ItemTickReset)
          (else
            (Default|CallInspectorUI (Variables|Default|GetFirst%20Person%20Tutorial) false)
            (Default|OBJDetach (Variables|Default|GetFirst%20Person%20Tutorial))))))))

(event Input|MouseEvents|LeftMouseButton
  (params (Key :type Key%20Structure :default "None"))
  (:Pressed
    (Variables|Default|SetbIsRotating true))
  (:Released
    (Variables|Default|SetbIsRotating false)))

(event Input|MouseEvents|MouseWheelUp
  (params (Key :type Key%20Structure :default "None"))
  (bind _scenecapturecomponent2d (Variables|Default|GetSceneCaptureComponent2D))
  (bind _relativelocation (Variables|/Script/Engine.SceneComponent|GetRelativeLocation _scenecapturecomponent2d))
  (:Pressed
    (Variables|Default|SetbReachZoomFloor false)
    (if (not (Variables|Default|GetbReachZoomCeiling))
      (Transformation|SetRelativeLocation (Variables|Default|GetSceneCaptureComponent2D) (Math|Vector|MakeVector (+ (Variables|Default|GetScale%20Units) (.x _relativelocation)) (.y _relativelocation) (.z _relativelocation)) false false)
      (if (>= (.x (Variables|/Script/Engine.SceneComponent|GetRelativeLocation (Variables|Default|GetSceneCaptureComponent2D))) (+ -7e+01 (* (Variables|Default|GetScale%20Units) 1e+01)))
        (Variables|Default|SetbReachZoomCeiling true)))))

(event Input|MouseEvents|MouseWheelDown
  (params (Key :type Key%20Structure :default "None"))
  (bind _scenecapturecomponent2d (Variables|Default|GetSceneCaptureComponent2D))
  (bind _relativelocation (Variables|/Script/Engine.SceneComponent|GetRelativeLocation _scenecapturecomponent2d))
  (:Pressed
    (Variables|Default|SetbReachZoomCeiling false)
    (if (not (Variables|Default|GetbReachZoomFloor))
      (Transformation|SetRelativeLocation (Variables|Default|GetSceneCaptureComponent2D) (Math|Vector|MakeVector (- (.x _relativelocation) (Variables|Default|GetScale%20Units)) (.y _relativelocation) (.z _relativelocation)) false false)
      (if (<= (.x (Variables|/Script/Engine.SceneComponent|GetRelativeLocation (Variables|Default|GetSceneCaptureComponent2D))) (+ -7e+01 (* (Variables|Default|GetScale%20Units) -1e+01)))
        (Variables|Default|SetbReachZoomFloor true)))))

(fn ConstructionScript)

(fn SetupInspectorData
  (bind _inspect_target (Variables|Default|GetInspect%20Target))
  (Utilities|FlowControl|Sequence
    (:then_0
      (Components|StaticMesh|SetStaticMesh (Variables|Default|GetItemToFocusMain) (Variables|/Script/Engine.StaticMeshComponent|GetStaticMesh (Variables|/Game/Project/Core/InteractOBJ/BP_CoreOBJ.BP_CoreOBJ_C|GetStaticMesh (Variables|Default|GetInspect%20Target)))))
    (:then_1
      (Transformation|SetRelativeTransform (Variables|Default|GetItemToFocusMain) (Variables|/Game/Project/Core/InteractOBJ/BP_CoreOBJ.BP_CoreOBJ_C|GetInspectorInitOffset (Variables|Default|GetInspect%20Target)) false false))
    (:then_2
      (CallFunction|ItemTickSetup (Variables|/Game/Project/Core/InteractOBJ/BP_CoreOBJ.BP_CoreOBJ_C|GetbTickWhenCheck _inspect_target) (Variables|/Game/Project/Core/InteractOBJ/BP_CoreOBJ.BP_CoreOBJ_C|GetOBJSerialCode _inspect_target)))))

(fn InitProjector
  (Transformation|SetRelativeLocation (Variables|Default|GetSceneCaptureComponent2D) "-70.000000,0.000000,0.000000" false false)
  (Variables|Default|SetbReachZoomCeiling false)
  (Variables|Default|SetbReachZoomFloor false))

(fn ItemTickSetup
  (params (bNeedTick :type Boolean) (OBJSerialCode :type Name))
  (bind _output_get (Variables|Default|SetbNeedTick bNeedTick))
  (if _output_get
    (Actor|Tick|SetActorTickEnabled true)
    (switch name OBJSerialCode
      (:K1002
        (Utilities|IsValid (Variables|Default|GetK1002_Liquid)
          (:Is%20Not%20Valid
            (bind _returnvalue (Rendering|Material|CreateDynamicMaterialInstance (Variables|Default|GetItemToFocusMain) 2 "/Game/Project/MaterialLibrary/MI_BottleLiquid2.MI_BottleLiquid2" "None" :!class /Script/Engine.PrimitiveComponent))
            (Variables|Default|SetK1002_Liquid _returnvalue)))))))

(fn ItemTickReset
  (bind _output_get (Variables|Default|SetbNeedTick false))
  (Actor|Tick|SetActorTickEnabled _output_get)
  (Variables|Default|SetLiquidWaveTime 0.0))

(fn SwitchInputMode
  (params (bEnterInspectMode :type Boolean))
  (bind _returnvalue (Game|GetPlayerController 0))
  (bind _returnvalue_2 (Game|GetPlayerController 0))
  (LocalVariables|SetL_EnterInspectMode bEnterInspectMode)
  (if (Variables|Default|GetbIsRegularStage)
    (LocalVariables|SetL_TargetPlayer (Variables|Default|GetFirst%20Person))
    (else
      (LocalVariables|SetL_TargetPlayer (Variables|Default|GetFirst%20Person%20Tutorial))))
  (if (LocalVariables|GetL_EnterInspectMode)
    (Input|DisableInput (LocalVariables|GetL_TargetPlayer) _returnvalue_2)
    (Input|EnableInput _returnvalue_2)
    (else
      (Input|DisableInput _returnvalue)
      (Input|EnableInput (LocalVariables|GetL_TargetPlayer) _returnvalue))))