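; BP_Studio_E is an item inspection studio that shows a given mesh to a SceneCapture2D for the player to examine.
; AssignInspectorData takes input from the regular or tutorial first-person character, sets up the mesh, resets zoom and raises the item by timeline.
; Left-drag rotates the item and the wheel moves the capture within limits.
; Right-click or IA_ItemCollection returns input, with slide-out and detach only for the tutorial character.
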(event Input|EnhancedActionEvents|EnhancedInputActionIA_ItemCollection
  (params (ActionValue :type Boolean) (ElapsedSeconds :type Float%20%28double-precision%29) (TriggeredSeconds :type Float%20%28double-precision%29) (InputAction :type Input%20Action%20Object%20Reference :default "/Game/ProjectDefault/FirstPerson/Input/Actions/IA_ItemCollection.IA_ItemCollection"))
  (bind _returnvalue (Game|GetPlayerController 0))
  (bind _returnvalue_2 (Game|GetPlayerController 0))
  (:Triggered
    (Utilities|IsValid (Variables|Default|GetFirst%20Person)
      (:Is%20Valid
        (Input|DisableInput _returnvalue)
        (Input|EnableInput (Variables|Default|GetFirst%20Person) _returnvalue))
      (:Is%20Not%20Valid
        (Utilities|IsValid (Variables|Default|GetFirst%20Person%20Tutorial)
          (:Is%20Valid
            (Input|DisableInput _returnvalue_2)
            (Input|EnableInput (Variables|Default|GetFirst%20Person%20Tutorial) _returnvalue_2)
            (bind _showingtrack (Timeline|Timeline ReverseFromEnd)
              (:Update
                (Transformation|SetRelativeLocation (Variables|Default|GetItemToFocus) (Math|Vector|Lerp(Vector) "0.000000,0.000000,-100.000000" "0, 0, 0" _showingtrack) false false))
              (:Finished
                (Default|CallInspectorUI (Variables|Default|GetFirst%20Person%20Tutorial) false)
                (Default|OBJDetach (Variables|Default|GetFirst%20Person%20Tutorial))))))))))

(event EventAssignInspectorData
  (params (ItemToFocus :type Static%20Mesh%20Object%20Reference) (InitRotation :type Rotator :default "0, 0, 0") (InitScale :type Vector :default "0, 0, 0") (FirstPerson :type BP%20First%20Person%20Character%20Object%20Reference) (FirstPersonTutorial :type BP%20First%20Person%20Character%20Tutorial%20Object%20Reference))
  (bind _returnvalue (Game|GetPlayerController 0))
  (bind _returnvalue_2 (Game|GetPlayerController 0))
  (Variables|Default|SetItem%20to%20Focus ItemToFocus)
  (Variables|Default|SetInit%20Rotation InitRotation)
  (Variables|Default|SetInit%20Scale InitScale)
  (Utilities|IsValid FirstPerson
    (:Is%20Valid
      (Variables|Default|SetFirst%20Person FirstPerson)
      (Input|DisableInput (Variables|Default|GetFirst%20Person) _returnvalue_2)
      (Input|EnableInput _returnvalue_2))
    (:Is%20Not%20Valid
      (Utilities|IsValid FirstPersonTutorial
        (:Is%20Valid
          (bind _output_get (Variables|Default|SetFirst%20Person%20Tutorial FirstPersonTutorial))
          (Default|CallInspectorUI _output_get true)
          (Input|DisableInput (Variables|Default|GetFirst%20Person%20Tutorial) _returnvalue)
          (Input|EnableInput _returnvalue)))))
  (CallFunction|SetupInspectorData)
  (CallFunction|InitProjector)
  (bind _showingtrack (Timeline|InspectorShowup PlayFromStart)
    (:Update
      (Transformation|SetRelativeLocation (Variables|Default|GetItemToFocus) (Math|Vector|Lerp(Vector) "0.000000,0.000000,-100.000000" "0, 0, 0" _showingtrack) false false))))

(event Input|MouseEvents|MouseX
  (params (AxisValue :type Float%20%28single-precision%29))
  (if (Variables|Default|GetbIsRotating)
    (Transformation|SetWorldRotation (Variables|Default|GetItemToFocus) (Math|Rotator|CombineRotators (Transformation|GetWorldRotation (Variables|Default|GetItemToFocus)) (Math|Rotator|MakeRotator 0.0 0.0 (* AxisValue -2.0))) false false)))

(event Input|MouseEvents|MouseY
  (params (AxisValue :type Float%20%28single-precision%29))
  (if (Variables|Default|GetbIsRotating)
    (Transformation|SetWorldRotation (Variables|Default|GetItemToFocus) (Math|Rotator|CombineRotators (Transformation|GetWorldRotation (Variables|Default|GetItemToFocus)) (Math|Rotator|MakeRotator 0.0 (* AxisValue -2.0) 0.0)) false false)))

(event Input|MouseEvents|RightMouseButton
  (params (Key :type Key%20Structure :default "None"))
  (bind _returnvalue (Game|GetPlayerController 0))
  (bind _returnvalue_2 (Game|GetPlayerController 0))
  (:Pressed
    (Utilities|IsValid (Variables|Default|GetFirst%20Person)
      (:Is%20Valid
        (Input|DisableInput _returnvalue)
        (Input|EnableInput (Variables|Default|GetFirst%20Person) _returnvalue))
      (:Is%20Not%20Valid
        (Utilities|IsValid (Variables|Default|GetFirst%20Person%20Tutorial)
          (:Is%20Valid
            (Input|DisableInput _returnvalue_2)
            (Input|EnableInput (Variables|Default|GetFirst%20Person%20Tutorial) _returnvalue_2)
            (bind _showingtrack (Timeline|Timeline ReverseFromEnd)
              (:Update
                (Transformation|SetRelativeLocation (Variables|Default|GetItemToFocus) (Math|Vector|Lerp(Vector) "0.000000,0.000000,-100.000000" "0, 0, 0" _showingtrack) false false))
              (:Finished
                (Default|CallInspectorUI (Variables|Default|GetFirst%20Person%20Tutorial) false)
                (Default|OBJDetach (Variables|Default|GetFirst%20Person%20Tutorial))))))))))

(event Input|MouseEvents|LeftMouseButton
  (params (Key :type Key%20Structure :default "None"))
  (:Pressed
    (Variables|Default|SetbIsRotating true))
  (:Released
    (Variables|Default|SetbIsRotating false)))

(event Input|MouseEvents|MouseWheelUp
  (params (Key :type Key%20Structure :default "None"))
  (bind _scenecapturecomponent2d (Variables|Default|GetSceneCaptureComponent2D))
  (bind _relativelocation (Variables|/Script/Engine.SceneComponent|GetRelativeLocation _scenecapturecomponent2d))
  (:Pressed
    (Variables|Default|SetbReachZoomFloor false)
    (if (not (Variables|Default|GetbReachZoomCeiling))
      (Transformation|SetRelativeLocation (Variables|Default|GetSceneCaptureComponent2D) (Math|Vector|MakeVector (+ 3.5 (.x _relativelocation)) (.y _relativelocation) (.z _relativelocation)) false false)
      (if (>= (.x (Variables|/Script/Engine.SceneComponent|GetRelativeLocation (Variables|Default|GetSceneCaptureComponent2D))) -35.0)
        (Variables|Default|SetbReachZoomCeiling true)))))

(event Input|MouseEvents|MouseWheelDown
  (params (Key :type Key%20Structure :default "None"))
  (bind _scenecapturecomponent2d (Variables|Default|GetSceneCaptureComponent2D))
  (bind _relativelocation (Variables|/Script/Engine.SceneComponent|GetRelativeLocation _scenecapturecomponent2d))
  (:Pressed
    (Variables|Default|SetbReachZoomCeiling false)
    (if (not (Variables|Default|GetbReachZoomFloor))
      (Transformation|SetRelativeLocation (Variables|Default|GetSceneCaptureComponent2D) (Math|Vector|MakeVector (+ -3.5 (.x _relativelocation)) (.y _relativelocation) (.z _relativelocation)) false false)
      (if (<= (.x (Variables|/Script/Engine.SceneComponent|GetRelativeLocation (Variables|Default|GetSceneCaptureComponent2D))) -105.0)
        (Variables|Default|SetbReachZoomFloor true)))))

(fn ConstructionScript)

(fn SetupInspectorData
  (Components|StaticMesh|SetStaticMesh (Variables|Default|GetItemToFocus) (Variables|Default|GetItem%20to%20Focus))
  (Transformation|SetRelativeRotation (Variables|Default|GetItemToFocus) (Variables|Default|GetInit%20Rotation) false false)
  (Transformation|SetRelativeScale3D (Variables|Default|GetItemToFocus) (Variables|Default|GetInit%20Scale)))

(fn InitProjector
  (Transformation|SetRelativeLocation (Variables|Default|GetSceneCaptureComponent2D) "-70.000000,0.000000,0.000000" false false)
  (Variables|Default|SetbReachZoomCeiling false)
  (Variables|Default|SetbReachZoomFloor false))

(fn AttachtoHand
  (params (InteractTarget :type Actor%20Component%20Object%20Reference))
  (return 0))

(fn ReturnExtractCode
  (return 0))

(fn ReturnOBJCode
  (return "None"))

(fn ReturnTRICKLists
  (return 0))