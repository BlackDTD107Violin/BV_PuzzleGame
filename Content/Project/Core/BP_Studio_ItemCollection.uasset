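; Item collection studio that shows a 3D item through a SceneCapture2D for inspection in the collection UI.
; AssignInspectorData sets the mesh and optional glass materials, moves input from the player to itself, and raises the item with a timeline.
; Mouse drag rotates the item, the wheel moves the capture within zoom limits, and keys drive HUD navigation.
; Closing lowers the item and restores input, branching between formal and tutorial characters.
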(event Input|EnhancedActionEvents|EnhancedInputActionIA_ItemCollectionInspector
  (params (ActionValue :type Boolean) (ElapsedSeconds :type Float%20%28double-precision%29) (TriggeredSeconds :type Float%20%28double-precision%29) (InputAction :type Input%20Action%20Object%20Reference :default "/Game/ProjectDefault/FirstPerson/Input/Actions/IA_ItemCollectionInspector.IA_ItemCollectionInspector"))
  (bind _returnvalue (Game|GetPlayerController 0))
  (bind _returnvalue_2 (Game|GetPlayerController 0))
  (bind _initlocation (Variables|Default|GetInitLocation))
  (bind _initlocation_2 (Variables|Default|GetInitLocation))
  (:Triggered
    (if (Variables|Default|GetbIsFormalMode)
      (Input|DisableInput _returnvalue)
      (Input|EnableInput (Variables|Default|GetFirst%20Person) _returnvalue)
      (bind _showingtrack (Timeline|Timeline_0 ReverseFromEnd)
        (:Update
          (Transformation|SetRelativeLocation (Variables|Default|GetItemToFocus) (Math|Vector|Lerp(Vector) (Math|Vector|MakeVector (.x _initlocation_2) (.y _initlocation_2) -1e+02) (Variables|Default|GetInitLocation) _showingtrack) false false))
        (:Finished
          (Default|CancelItemCollectionUI (Variables|Default|GetFirst%20Person))
          (Default|ToggleItemList (Variables|/Game/ProjectDefault/FirstPerson/Blueprints/BP_FirstPersonCharacter.BP_FirstPersonCharacter_C|GetREF_CoreHUD (Variables|Default|GetFirst%20Person)))))
      (else
        (Input|DisableInput _returnvalue_2)
        (Input|EnableInput (Variables|Default|GetFirst%20Person%20Tutorial) _returnvalue_2)
        (bind _showingtrack_2 (Timeline|Timeline ReverseFromEnd)
          (:Update
            (Transformation|SetRelativeLocation (Variables|Default|GetItemToFocus) (Math|Vector|Lerp(Vector) (Math|Vector|MakeVector (.x _initlocation) (.y _initlocation) -1e+02) (Variables|Default|GetInitLocation) _showingtrack_2) false false))
          (:Finished
            (Default|CancelItemCollectionUI (Variables|Default|GetFirst%20Person%20Tutorial))
            (Default|ToggleItemList (Variables|/Game/ProjectDefault/FirstPerson/Blueprints/BP_FirstPersonCharacterTutorial.BP_FirstPersonCharacterTutorial_C|GetREF_CoreHUDTutorial (Variables|Default|GetFirst%20Person%20Tutorial)))))))))

(event Input|EnhancedActionEvents|EnhancedInputActionIA_ItemCollectionPage
  (params (ActionValue :type Boolean) (ElapsedSeconds :type Float%20%28double-precision%29) (TriggeredSeconds :type Float%20%28double-precision%29) (InputAction :type Input%20Action%20Object%20Reference :default "/Game/ProjectDefault/FirstPerson/Input/Actions/IA_ItemCollectionPage.IA_ItemCollectionPage"))
  (:Triggered
    (if (Variables|Default|GetbIsFormalMode)
      (Default|SwitchItemPageCollection (Variables|/Game/ProjectDefault/FirstPerson/Blueprints/BP_FirstPersonCharacter.BP_FirstPersonCharacter_C|GetREF_CoreHUD (Variables|Default|GetFirst%20Person))))))

(event Input|EnhancedActionEvents|EnhancedInputActionIA_ItemCollectionTag
  (params (ActionValue :type Boolean) (ElapsedSeconds :type Float%20%28double-precision%29) (TriggeredSeconds :type Float%20%28double-precision%29) (InputAction :type Input%20Action%20Object%20Reference :default "/Game/ProjectDefault/FirstPerson/Input/Actions/IA_ItemCollectionTag.IA_ItemCollectionTag"))
  (:Triggered
    (if (and (not (Variables|/Game/ProjectDefault/FirstPerson/Blueprints/BP_FirstPersonCharacter.BP_FirstPersonCharacter_C|GetbIgnoreTab (Variables|Default|GetFirst%20Person))) (Variables|Default|GetbIsFormalMode))
      (Default|SwitchItemTagCollection (Variables|/Game/ProjectDefault/FirstPerson/Blueprints/BP_FirstPersonCharacter.BP_FirstPersonCharacter_C|GetREF_CoreHUD (Variables|Default|GetFirst%20Person))))))

(event Input|EnhancedActionEvents|EnhancedInputActionIA_GlassDiscard
  (params (ActionValue :type Boolean) (ElapsedSeconds :type Float%20%28double-precision%29) (TriggeredSeconds :type Float%20%28double-precision%29) (InputAction :type Input%20Action%20Object%20Reference :default "/Game/ProjectDefault/FirstPerson/Input/Actions/IA_GlassDiscard.IA_GlassDiscard"))
  (:Triggered
    (Default|RequestGlassDiscard (Variables|/Game/ProjectDefault/FirstPerson/Blueprints/BP_FirstPersonCharacter.BP_FirstPersonCharacter_C|GetREF_CoreHUD (Variables|Default|GetFirst%20Person)))))

(event EventBeginPlay
  (Utilities|Casting|CastToBP_FirstPersonCharacter (Game|GetPlayerCharacter 0)
    (:then
      (Variables|Default|SetbIsFormalMode true))
    (:CastFailed
      (Variables|Default|SetbIsFormalMode false))))

(event EventGlassMatModify
  (params (bGlaaIsUnite :type Boolean) (DiamondMats :type Array%20of%20Material%20Instance%20Dynamic%20Object%20References) (TotemMats :type Material%20Interface%20Object%20Reference))
  (if bGlaaIsUnite
    (for (_array_element _array_index) DiamondMats
      (Rendering|Material|SetMaterial (Variables|Default|GetItemToFocus) (+ _array_index 4) _array_element)
      (Rendering|Material|SetMaterial (Variables|Default|GetItemToFocus) 3 TotemMats))
    (else
      (Rendering|Material|SetMaterial (Variables|Default|GetItemToFocus) 3 TotemMats))))

(event EventAssignInspectorData
  (params (ItemToFocus :type Static%20Mesh%20Object%20Reference) (InitOffset :type Transform) (ScaleUnits :type Float%20%28double-precision%29) (FirstPerson :type BP%20First%20Person%20Character%20Object%20Reference) (FirstPersonTutorial :type BP%20First%20Person%20Character%20Tutorial%20Object%20Reference) (bIsGlass :type Boolean) (bGlassIsUnite :type Boolean) (GlassDiamondMats :type Array%20of%20Material%20Instance%20Dynamic%20Object%20References) (TotemMat :type Material%20Interface%20Object%20Reference))
  (bind _returnvalue (Game|GetPlayerController 0))
  (bind _returnvalue_2 (Game|GetPlayerController 0))
  (Variables|Default|SetItem%20to%20Focus ItemToFocus)
  (bind _output_get (Variables|Default|SetInit%20Offset InitOffset))
  (Variables|Default|SetInitLocation (.location _output_get))
  (Variables|Default|SetScale%20Units ScaleUnits)
  (if bIsGlass
    (CallFunction|GlassMatModify bGlassIsUnite GlassDiamondMats TotemMat))
  (if (Variables|Default|GetbIsFormalMode)
    (Variables|Default|SetFirst%20Person FirstPerson)
    (Input|DisableInput (Variables|Default|GetFirst%20Person) _returnvalue_2)
    (Input|EnableInput _returnvalue_2)
    (else
      (Variables|Default|SetFirst%20Person%20Tutorial FirstPersonTutorial)
      (Input|DisableInput (Variables|Default|GetFirst%20Person%20Tutorial) _returnvalue)
      (Input|EnableInput _returnvalue)))
  (CallFunction|SetupInspectorData)
  (CallFunction|InitProjector)
  (bind _showingtrack (Timeline|InspectorShowup PlayFromStart)
    (:Update
      (Transformation|SetRelativeLocation (Variables|Default|GetItemToFocus) (Math|Vector|Lerp(Vector) (Math|Vector|MakeVector (.x (Variables|Default|GetInitLocation)) (.y (Variables|Default|GetInitLocation)) -1e+02) (Variables|Default|GetInitLocation) _showingtrack) false false))))

(event Input|MouseEvents|MouseX
  (params (AxisValue :type Float%20%28single-precision%29))
  (if (Variables|Default|GetbIsRotating)
    (Transformation|SetWorldRotation (Variables|Default|GetItemToFocus) (Math|Rotator|CombineRotators (Transformation|GetWorldRotation (Variables|Default|GetItemToFocus)) (Math|Rotator|MakeRotator 0.0 0.0 (* AxisValue -2.0))) false false)))

(event Input|MouseEvents|MouseY
  (params (AxisValue :type Float%20%28single-precision%29))
  (if (Variables|Default|GetbIsRotating)
    (Transformation|SetWorldRotation (Variables|Default|GetItemToFocus) (Math|Rotator|CombineRotators (Transformation|GetWorldRotation (Variables|Default|GetItemToFocus)) (Math|Rotator|MakeRotator 0.0 (* AxisValue -2.0) 0.0)) false false)))

(event Input|KeyboardEvents|W
  (params (Key :type Key%20Structure :default "None"))
  (:Pressed
    (if (Variables|Default|GetbIsFormalMode)
      (Default|MoveCurrentFocus (Variables|/Game/ProjectDefault/FirstPerson/Blueprints/BP_FirstPersonCharacter.BP_FirstPersonCharacter_C|GetREF_CoreHUD (Variables|Default|GetFirst%20Person)) -1))))

(event Input|KeyboardEvents|A
  (params (Key :type Key%20Structure :default "None"))
  (:Pressed
    (if (Variables|Default|GetbIsFormalMode)
      (Default|MoveCurrentFocus (Variables|/Game/ProjectDefault/FirstPerson/Blueprints/BP_FirstPersonCharacter.BP_FirstPersonCharacter_C|GetREF_CoreHUD (Variables|Default|GetFirst%20Person)) -5))))

(event Input|KeyboardEvents|S
  (params (Key :type Key%20Structure :default "None"))
  (:Pressed
    (if (Variables|Default|GetbIsFormalMode)
      (Default|MoveCurrentFocus (Variables|/Game/ProjectDefault/FirstPerson/Blueprints/BP_FirstPersonCharacter.BP_FirstPersonCharacter_C|GetREF_CoreHUD (Variables|Default|GetFirst%20Person)) 1))))

(event Input|KeyboardEvents|D
  (params (Key :type Key%20Structure :default "None"))
  (:Pressed
    (if (Variables|Default|GetbIsFormalMode)
      (Default|MoveCurrentFocus (Variables|/Game/ProjectDefault/FirstPerson/Blueprints/BP_FirstPersonCharacter.BP_FirstPersonCharacter_C|GetREF_CoreHUD (Variables|Default|GetFirst%20Person)) 5))))

(event Input|MouseEvents|RightMouseButton
  (params (Key :type Key%20Structure :default "None"))
  (bind _returnvalue (Game|GetPlayerController 0))
  (bind _returnvalue_2 (Game|GetPlayerController 0))
  (bind _initlocation (Variables|Default|GetInitLocation))
  (bind _initlocation_2 (Variables|Default|GetInitLocation))
  (:Pressed
    (if (Variables|Default|GetbIsFormalMode)
      (Input|DisableInput _returnvalue)
      (Input|EnableInput (Variables|Default|GetFirst%20Person) _returnvalue)
      (bind _showingtrack (Timeline|Timeline_0 ReverseFromEnd)
        (:Update
          (Transformation|SetRelativeLocation (Variables|Default|GetItemToFocus) (Math|Vector|Lerp(Vector) (Math|Vector|MakeVector (.x _initlocation_2) (.y _initlocation_2) -1e+02) (Variables|Default|GetInitLocation) _showingtrack) false false))
        (:Finished
          (Default|CancelItemCollectionUI (Variables|Default|GetFirst%20Person))
          (Default|ToggleItemList (Variables|/Game/ProjectDefault/FirstPerson/Blueprints/BP_FirstPersonCharacter.BP_FirstPersonCharacter_C|GetREF_CoreHUD (Variables|Default|GetFirst%20Person)))))
      (else
        (Input|DisableInput _returnvalue_2)
        (Input|EnableInput (Variables|Default|GetFirst%20Person%20Tutorial) _returnvalue_2)
        (bind _showingtrack_2 (Timeline|Timeline ReverseFromEnd)
          (:Update
            (Transformation|SetRelativeLocation (Variables|Default|GetItemToFocus) (Math|Vector|Lerp(Vector) (Math|Vector|MakeVector (.x _initlocation) (.y _initlocation) -1e+02) (Variables|Default|GetInitLocation) _showingtrack_2) false false))
          (:Finished
            (Default|CancelItemCollectionUI (Variables|Default|GetFirst%20Person%20Tutorial))
            (Default|ToggleItemList (Variables|/Game/ProjectDefault/FirstPerson/Blueprints/BP_FirstPersonCharacterTutorial.BP_FirstPersonCharacterTutorial_C|GetREF_CoreHUDTutorial (Variables|Default|GetFirst%20Person%20Tutorial)))))))))

(event Input|MouseEvents|LeftMouseButton
  (params (Key :type Key%20Structure :default "None"))
  (:Pressed
    (Variables|Default|SetbIsRotating true))
  (:Released
    (Variables|Default|SetbIsRotating false)))

(event Input|MouseEvents|MouseWheelUp
  (params (Key :type Key%20Structure :default "None"))
  (bind _scenecapturecomponent2d (Variables|Default|GetSceneCaptureComponent2D))
  (bind _relativelocation (Variables|/Script/Engine.SceneComponent|GetRelativeLocation _scenecapturecomponent2d))
  (:Pressed
    (Variables|Default|SetbReachZoomFloor false)
    (if (not (Variables|Default|GetbReachZoomCeiling))
      (Transformation|SetRelativeLocation (Variables|Default|GetSceneCaptureComponent2D) (Math|Vector|MakeVector (+ (Variables|Default|GetScale%20Units) (.x _relativelocation)) (.y _relativelocation) (.z _relativelocation)) false false)
      (if (>= (.x (Variables|/Script/Engine.SceneComponent|GetRelativeLocation (Variables|Default|GetSceneCaptureComponent2D))) (+ -7e+01 (* (Variables|Default|GetScale%20Units) 1e+01)))
        (Variables|Default|SetbReachZoomCeiling true)))))

(event Input|MouseEvents|MouseWheelDown
  (params (Key :type Key%20Structure :default "None"))
  (bind _scenecapturecomponent2d (Variables|Default|GetSceneCaptureComponent2D))
  (bind _relativelocation (Variables|/Script/Engine.SceneComponent|GetRelativeLocation _scenecapturecomponent2d))
  (:Pressed
    (Variables|Default|SetbReachZoomCeiling false)
    (if (not (Variables|Default|GetbReachZoomFloor))
      (Transformation|SetRelativeLocation (Variables|Default|GetSceneCaptureComponent2D) (Math|Vector|MakeVector (- (.x _relativelocation) (Variables|Default|GetScale%20Units)) (.y _relativelocation) (.z _relativelocation)) false false)
      (if (<= (.x (Variables|/Script/Engine.SceneComponent|GetRelativeLocation (Variables|Default|GetSceneCaptureComponent2D))) (+ -7e+01 (* (Variables|Default|GetScale%20Units) -1e+01)))
        (Variables|Default|SetbReachZoomFloor true)))))

(fn ConstructionScript)

(fn SetupInspectorData
  (Components|StaticMesh|SetStaticMesh (Variables|Default|GetItemToFocus) (Variables|Default|GetItem%20to%20Focus))
  (Transformation|SetRelativeTransform (Variables|Default|GetItemToFocus) (Variables|Default|GetInit%20Offset) false false))

(fn InitProjector
  (Transformation|SetRelativeLocation (Variables|Default|GetSceneCaptureComponent2D) "-70.000000,0.000000,0.000000" false false)
  (Variables|Default|SetbReachZoomCeiling false)
  (Variables|Default|SetbReachZoomFloor false))

(fn AttachtoHand
  (params (InteractTarget :type Actor%20Component%20Object%20Reference))
  (return 0))

(fn ReturnExtractCode
  (return 0))

(fn ReturnOBJCode
  (return "None"))

(fn ReturnTRICKLists
  (return 0))