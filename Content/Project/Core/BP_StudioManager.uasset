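; Manager that sets up off-world studio actors for inspecting, listing and dragging items and glass.
; Call events lazily spawn and reuse one studio per use at far-off coordinates, then pass it the target, glass flags and materials.
; For glass it reads the totem material; Unite glass also animates three shared diamond dynamic materials according to its inherit layer.
; Both Close events set their studio's HiddenInGame to false, leaving it visible.
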(event Custom|CallStudio
  (params (InspectTarget :type BP%20Core%20OBJ%20Object%20Reference))
  ;[1 1 1] Call Studio Item - Inspect Item
  (Variables|Default|SetInspectTarget InspectTarget)
  (Utilities|FlowControl|Sequence
    (:then_0
      (Utilities|IsValid (Variables|Default|GetREF_Studio)
        (:Is%20Not%20Valid
          (bind _returnvalue (Game|SpawnActorfromClass "/Game/Project/Core/BP_Studio.BP_Studio_C" (Math|Transform|MakeTransform "1000000000.000000,0.000000,0.000000") "Undefined" 0 0))
          (Variables|Default|SetREF_Studio _returnvalue))))
    (:then_1
      (CallFunction|AssignTargetData (Variables|Default|GetInspectTarget))
      (Class|BICoreOBJInteractInterface|AssignInspectorData(Message) (Variables|Default|GetREF_Studio) (Variables|Default|GetInspectTarget) (Variables|Default|GetbIsGlass) (Variables|Default|GetbGlassIsUnite) (Variables|Default|GetDiamondGroups) (Variables|Default|GetTotemMats)))))

(event Custom|CloseStudio
  ;[1 1 1] Call Studio Item - Inspect Item
  (Rendering|SetActorHiddenInGame (Variables|Default|GetREF_Studio) false))

(event Custom|CallStudio_ItemCollection
  (params (InspectTarget :type BP%20Core%20OBJ%20Object%20Reference))
  ;[1 1 1] Call Studio Item - Item List
  (Variables|Default|SetInspectTarget InspectTarget)
  (Utilities|FlowControl|Sequence
    (:then_0
      (Utilities|IsValid (Variables|Default|GetREF_Studio_E)
        (:Is%20Not%20Valid
          (bind _returnvalue (Game|SpawnActorfromClass "/Game/Project/Core/BP_Studio_ItemCollection.BP_Studio_ItemCollection_C" (Math|Transform|MakeTransform "1000000000.000000,0.000000,1000000000.000000") "Undefined" 0 0))
          (Variables|Default|SetREF_Studio_E _returnvalue))))
    (:then_1
      (CallFunction|AssignTargetData (Variables|Default|GetInspectTarget))
      (Class|BICoreOBJInteractInterface|AssignInspectorData(Message) (Variables|Default|GetREF_Studio_E) (Variables|Default|GetInspectTarget) (Variables|Default|GetbIsGlass) (Variables|Default|GetbGlassIsUnite) (Variables|Default|GetDiamondGroups) (Variables|Default|GetTotemMats)))))

(event Custom|CloseStudio_ItemCollection
  ;[1 1 1] Call Studio Item - Item List
  (Rendering|SetActorHiddenInGame (Variables|Default|GetREF_Studio_E) false))

(event Custom|CallStudio_ItemCollection_ButEmpty
  ;[1 1 1] Call Studio Item - Item List
  (Utilities|FlowControl|Sequence
    (:then_0
      (Utilities|IsValid (Variables|Default|GetREF_Studio_E)
        (:Is%20Not%20Valid
          (bind _returnvalue (Game|SpawnActorfromClass "/Game/Project/Core/BP_Studio_ItemCollection.BP_Studio_ItemCollection_C" (Math|Transform|MakeTransform "1000000000.000000,0.000000,1000000000.000000") "Undefined" 0 0))
          (Variables|Default|SetREF_Studio_E _returnvalue))))
    (:then_1
      (Class|BICoreOBJInteractInterface|AssignInspectorData(Message) (Variables|Default|GetREF_Studio_E) 0 (Variables|Default|GetbIsGlass) (Variables|Default|GetbGlassIsUnite) (Variables|Default|GetDiamondGroups) (Variables|Default|GetTotemMats)))))

(event Custom|CallStudio_GlassBaseDrag
  (params (GlassType :type E_GLASSType%20Enum :default "NewEnumerator6") (Target%20Valid%20Data%20Base :type ST%20Glass%20Data%20Structure) (Target%20Valid%20Data%20Unite :type ST%20Glass%20Data%20Structure))
  (switch Utilities|FlowControl|Switch|SwitchonE_GLASSType GlassType
    (:NewEnumerator6
      (Variables|Default|SetInspectTarget (Utilities|Struct|BreakST_GlassData Target%20Valid%20Data%20Base)))
    (:NewEnumerator1
      (Variables|Default|SetInspectTarget (Utilities|Struct|BreakST_GlassData Target%20Valid%20Data%20Unite))))
  (Utilities|FlowControl|Sequence
    (:then_0
      (Utilities|IsValid (Variables|Default|GetREF_Studio_DD)
        (:Is%20Not%20Valid
          (bind _returnvalue (Game|SpawnActorfromClass "/Game/Project/Core/BP_Studio_DD.BP_Studio_DD_C" (Math|Transform|MakeTransform "1000000000.000000,0.000000,2000000000.000000") "Undefined" 0 0))
          (Variables|Default|SetREF_Studio_DD _returnvalue))))
    (:then_1
      (CallFunction|AssignTargetData (Variables|Default|GetInspectTarget))
      (Class|BICoreOBJInteractInterface|AssignInspectorData(Message) (Variables|Default|GetREF_Studio_DD) (Variables|Default|GetInspectTarget) (Variables|Default|GetbIsGlass) (Variables|Default|GetbGlassIsUnite) (Variables|Default|GetDiamondGroups) (Variables|Default|GetTotemMats)))))

(event Custom|CallStudio_GlassCollection
  (params (InspectTarget :type BP%20Core%20OBJ%20Object%20Reference))
  (Variables|Default|SetInspectTarget InspectTarget)
  (Utilities|FlowControl|Sequence
    (:then_0
      (Utilities|IsValid (Variables|Default|GetREF_Studio_E)
        (:Is%20Not%20Valid
          (bind _returnvalue (Game|SpawnActorfromClass "/Game/Project/Core/BP_Studio_ItemCollection.BP_Studio_ItemCollection_C" (Math|Transform|MakeTransform "1000000000.000000,0.000000,1000000000.000000") "Undefined" 0 0))
          (Variables|Default|SetREF_Studio_E _returnvalue))))
    (:then_1
      (CallFunction|AssignTargetData (Variables|Default|GetInspectTarget))
      (Class|BICoreOBJInteractInterface|AssignInspectorData(Message) (Variables|Default|GetREF_Studio_E) (Variables|Default|GetInspectTarget) (Variables|Default|GetbIsGlass) (Variables|Default|GetbGlassIsUnite) (Variables|Default|GetDiamondGroups) (Variables|Default|GetTotemMats)))))

(event Custom|CallStudio_ItemDrag
  (params (Target%20Valid%20Data :type ST%20Item%20Collection%20Structure))
  ;[1 1 1] Call Studio Item - Drag Item
  (bind _asbp_core_obj (Utilities|Casting|CastToBP_CoreOBJ (Utilities|Struct|BreakST_ItemCollection Target%20Valid%20Data)))
  (Variables|Default|SetInspectTarget _asbp_core_obj)
  (Utilities|FlowControl|Sequence
    (:then_0
      (Utilities|IsValid (Variables|Default|GetREF_Studio_DD)
        (:Is%20Not%20Valid
          (bind _returnvalue (Game|SpawnActorfromClass "/Game/Project/Core/BP_Studio_DD.BP_Studio_DD_C" (Math|Transform|MakeTransform "1000000000.000000,0.000000,2000000000.000000") "Undefined" 0 0))
          (Variables|Default|SetREF_Studio_DD _returnvalue))))
    (:then_1
      (CallFunction|AssignTargetData (Variables|Default|GetInspectTarget))
      (Class|BICoreOBJInteractInterface|AssignInspectorData(Message) (Variables|Default|GetREF_Studio_DD) (Variables|Default|GetInspectTarget) (Variables|Default|GetbIsGlass) (Variables|Default|GetbGlassIsUnite) (Variables|Default|GetDiamondGroups) (Variables|Default|GetTotemMats)))))

(event EventBeginPlay
  (CallFunction|CreateDiamondMat))

(fn ConstructionScript)

(fn AssignTargetData
  (params (TargetInspect :type BP%20Core%20OBJ%20Object%20Reference))
  (bind _output_get (LocalVariables|SetL_TargetInspect TargetInspect))
  (bind _asbp_glassitem (Utilities|Casting|CastToBP_GLASSItem _output_get)
    (:then
      (Variables|Default|SetbIsGlass true)
      (Variables|Default|SetTotemMats (Rendering|Material|GetMaterial (Variables|/Game/Project/Core/InteractOBJ/BP_CoreOBJ.BP_CoreOBJ_C|GetStaticMesh _asbp_glassitem) 3))
      (bind _output_get_2 (Variables|Default|SetbGlassIsUnite (Utilities|Enum|Equal(Enum) (Variables|/Game/Project/Core/InteractOBJ/BP_CoreOBJ_GLASS.BP_CoreOBJ_GLASS_C|GetGlassType _asbp_glassitem) "NewEnumerator1")))
      (if _output_get_2
        (CallFunction|SetInheritDiamond _asbp_glassitem)))
    (:CastFailed
      (Variables|Default|SetbIsGlass false)
      (Variables|Default|SetbGlassIsUnite false)))
  (return))

(fn SetInheritDiamond
  (params (UniteGlass :type BP%20GLASS%20Item%20Object%20Reference))
  (LocalVariables|SetL_Layer (.inheritlayer (Variables|/Game/Project/InteractOBJ/BP_GLASSItem.BP_GLASSItem_C|GetThisGlass UniteGlass)))
  (for _index (range 0 2)
    (bind _output_get (LocalVariables|SetL_LoopIndex _index))
    (if (< _output_get (LocalVariables|GetL_Layer))
      (Rendering|Material|SetScalarParameterValue (Utilities|Array|Get(acopy) (Variables|Default|GetDiamondGroups) (LocalVariables|GetL_LoopIndex)) "Enable" 1.0 :!class /Script/Engine.MaterialInstanceDynamic)
      (Rendering|Material|SetScalarParameterValue (Utilities|Array|Get(acopy) (Variables|Default|GetDiamondGroups) (LocalVariables|GetL_LoopIndex)) "Speed" 0.1 :!class /Script/Engine.MaterialInstanceDynamic)
      (else
        (Rendering|Material|SetScalarParameterValue (Utilities|Array|Get(acopy) (Variables|Default|GetDiamondGroups) (LocalVariables|GetL_LoopIndex)) "Enable" 0.0 :!class /Script/Engine.MaterialInstanceDynamic)
        (Rendering|Material|SetScalarParameterValue (Utilities|Array|Get(acopy) (Variables|Default|GetDiamondGroups) (LocalVariables|GetL_LoopIndex)) "Speed" 0.0 :!class /Script/Engine.MaterialInstanceDynamic)))))

(fn CreateDiamondMat
  (Utilities|FlowControl|Sequence
    (:then_0
      (bind _returnvalue (Rendering|Material|CreateDynamicMaterialInstance "/Game/Project/Artist/KeyObj/Material/Slider_Diamond00.Slider_Diamond00" "None" "None" :!class /Script/Engine.KismetMaterialLibrary))
      (bind _output_get (Variables|Default|SetDiamond_L _returnvalue))
      (Utilities|Array|Add (Variables|Default|GetDiamondGroups) _output_get))
    (:then_1
      (bind _returnvalue_2 (Rendering|Material|CreateDynamicMaterialInstance "/Game/Project/Artist/KeyObj/Material/Slider_Diamond02.Slider_Diamond02" "None" "None" :!class /Script/Engine.KismetMaterialLibrary))
      (bind _output_get_2 (Variables|Default|SetDiamond_R _returnvalue_2))
      (Utilities|Array|Add (Variables|Default|GetDiamondGroups) _output_get_2))
    (:then_2
      (bind _returnvalue_3 (Rendering|Material|CreateDynamicMaterialInstance "/Game/Project/Artist/KeyObj/Material/Slider_Diamond01.Slider_Diamond01" "None" "None" :!class /Script/Engine.KismetMaterialLibrary))
      (bind _output_get_3 (Variables|Default|SetDiamond_M _returnvalue_3))
      (Utilities|Array|Add (Variables|Default|GetDiamondGroups) _output_get_3))
    (:then_3
      (for _array_element (Variables|Default|GetDiamondGroups)
        (Rendering|Material|SetScalarParameterValue _array_element "Enable" 0.0 :!class /Script/Engine.MaterialInstanceDynamic)
        (Rendering|Material|SetScalarParameterValue _array_element "Speed" 0.0 :!class /Script/Engine.MaterialInstanceDynamic)))))