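; BP_SET_GLASSplace_Machine is an interactable slot, expected as a child actor of BP_GlassCalculateMachine, where the player places glass objects.
; On interact it checks that the object is a BP_CoreOBJ_GLASS of the matching glass type.
; A match has the player assign it to the slot's PlaceLocation and passes its glass code to the parent machine.
; A wrong type or other object opens a corresponding player dialogue.
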(event EventBeginPlay
  (bind _returnvalue (Actor|GetParentActor))
  (|CallParentFunction)
  (bind _asbp_first_person_character (Utilities|Casting|CastToBP_FirstPersonCharacter (Game|GetPlayerCharacter 0)))
  (Variables|Default|SetPlayer _asbp_first_person_character)
  (Utilities|IsValid _returnvalue
    (:Is%20Valid
      (bind _asbp_glass_calculate_machine (Utilities|Casting|CastToBP_GlassCalculateMachine _returnvalue))
      (Variables|Default|SetREF_GlassCalculateMachine _asbp_glass_calculate_machine))))

(event EventInteract
  (params (InteractActor :type Actor%20Object%20Reference) (InteractTarget :type Actor%20Component%20Object%20Reference))
  (bind _asbp_core_obj_glass (Utilities|Casting|CastToBP_CoreOBJ_GLASS InteractActor)
    (:then
      (bind _output_get (Variables|Default|SetREF_InsertedGLASS _asbp_core_obj_glass))
      (if (Utilities|Enum|Equal(Enum) (Variables|Default|GetMatchGlassType) (Variables|/Game/Project/Core/InteractOBJ/BP_CoreOBJ_GLASS.BP_CoreOBJ_GLASS_C|GetGlassType _output_get))
        (Default|OBJAssigntoSET (Variables|Default|GetPlayer) (Transformation|GetWorldLocation (Variables|Default|GetPlaceLocation)) self)
        (Variables|Default|SetbHavePlacedOBJ true)
        (Default|ReceiveGLASSCode (Variables|Default|GetREF_GlassCalculateMachine) (Variables|/Game/Project/Core/InteractOBJ/BP_CoreOBJ_GLASS.BP_CoreOBJ_GLASS_C|GetThisGlass (Variables|Default|GetREF_InsertedGLASS)))
        (else
          (Default|OpenDialogueTA (Variables|Default|GetPlayer) "800003"))))
    (:CastFailed
      (Default|OpenDialogueTA (Variables|Default|GetPlayer) "800002"))))

(fn ConstructionScript
  (|CallParentFunction))