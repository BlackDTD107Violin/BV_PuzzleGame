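; BP_CoreITEM_GLASS is an interactable glass item that reacts to entering and exiting an inspector view.
; Entering plays the interact sound attached to its static mesh and hides that mesh.
; Exiting plays the sound again, then hides the whole actor and disables its collision without destroying it.
; Its construction script only calls the parent's.
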(event EventEnterInspector
  (Audio|SpawnSoundAttached (Variables|Default|GetInteractSE) (Variables|Default|GetStaticMesh) "None" "0, 0, 0" "0, 0, 0" "KeepRelativeOffset" false 1.0 1.0 0.0 0 0)
  (Development|SetHiddeninGame (Variables|Default|GetStaticMesh) true false))

(event EventExitInspector
  (Audio|SpawnSoundAttached (Variables|Default|GetInteractSE) (Variables|Default|GetStaticMesh) "None" "0, 0, 0" "0, 0, 0" "KeepRelativeOffset" false 1.0 1.0 0.0 0 0)
  (Rendering|SetActorHiddenInGame true)
  (Collision|SetActorEnableCollision false))

(fn ConstructionScript
  (|CallParentFunction))