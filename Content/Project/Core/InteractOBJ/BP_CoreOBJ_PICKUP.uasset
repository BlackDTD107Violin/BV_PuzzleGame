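; BP_CoreOBJ_PICKUP is a core interact-object Blueprint for pickups, layered on a parent class's construction script.
; BeginPlay tags it with an object-type enum value.
; SetupParent_0 caches the actor's original transform and flags whether it has a valid parent actor.
; The serial-code and extract-code getters return only empty defaults.
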(event EventBeginPlay
  (Variables|Default|SetThisOBJtype "NewEnumerator2"))

(fn ConstructionScript
  (|CallParentFunction))

(fn SetupParent0
  (Variables|Default|SetOriginalPos_0 (Transformation|GetActorTransform))
  (Utilities|IsValid (Actor|GetParentActor)
    (:Is%20Valid
      (Variables|Default|SetbHasParent_0 true))))

(fn ReturnPICKUPCode
  (return "None" 0))

(fn ReturnExtractCode
  (return 0))