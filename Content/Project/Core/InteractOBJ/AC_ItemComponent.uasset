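; Item component for interactable objects that handles interaction sound, mesh visibility and an extract material effect.
; On interaction it plays a sound attached to the given mesh and hides it when entering the state.
; On leaving, the mesh is shown again only if the item cannot be stored in a slot.
; A separate function drives a LerpAlpha scalar across the extract material group for blending.
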(fn SetExtractMatVal
  (params (LerpVal :type Float%20%28double-precision%29))
  (for _array_element (Variables|Default|GetExtractMatgroups)
    (Rendering|Material|SetScalarParameterValue _array_element "LerpAlpha" LerpVal :!class /Script/Engine.MaterialInstanceDynamic)))

(fn SpawnSEandSetMeshHidden
  (params (SelfSM :type Static%20Mesh%20Component%20Object%20Reference) (bIsEnterState :type Boolean))
  (LocalVariables|SetL_SelfSM SelfSM)
  (LocalVariables|SetIsEnterState bIsEnterState)
  (Audio|SpawnSoundAttached (Variables|Default|GetInteractSE) (LocalVariables|GetL_SelfSM) "None" "0, 0, 0" "0, 0, 0" "KeepRelativeOffset" false 1.0 1.0 0.0 0 0)
  (if (LocalVariables|GetIsEnterState)
    (Development|SetHiddeninGame (LocalVariables|GetL_SelfSM) (LocalVariables|GetIsEnterState) false :!label _label)
    (elif (not (Variables|Default|GetbCanStoreInSlot))
      (goto _label))))