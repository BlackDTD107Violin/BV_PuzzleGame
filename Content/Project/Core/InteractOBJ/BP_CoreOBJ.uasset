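; BP_CoreOBJ is a core interactable object Blueprint that exposes query functions for object type, hand attachment, codes and trick lists.
; SetupParent stores the actor's starting transform and flags whether it has a valid parent actor.
; The type and attach queries return member variables, while the extract code, object code and trick list queries return only placeholder defaults.
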(fn ConstructionScript)

(fn SetupParent
  (Variables|Default|SetOriginalPos (Transformation|GetActorTransform))
  (Utilities|IsValid (Actor|GetParentActor)
    (:Is%20Valid
      (Variables|Default|SetbHasParent true))))

(fn ReturnOBJType
  (return (Variables|Default|GetThisOBJtype)))

(fn AttachtoHand
  (params (InteractTarget :type Actor%20Component%20Object%20Reference))
  (return (Variables|Default|GetCurrentAttachSET)))

(fn ReturnExtractCode
  (return 0))

(fn ReturnOBJCode
  (return "None"))

(fn ReturnTRICKLists
  (return 0))