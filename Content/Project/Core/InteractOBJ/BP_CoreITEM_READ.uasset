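; BP_CoreITEM_READ is an interactable item, apparently a readable one, that reacts to entering and exiting an inspector view.
; On enter, it plays InteractSE attached to its StaticMesh and hides the mesh.
; On exit, it replays the sound and uses CanBeStored to either keep the item hidden without collision or show it again with collision.
; The construction script only calls the parent, and an actor-level hide and collision-off chain is left unconnected.
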(event EventEnterInspector
  (Audio|SpawnSoundAttached (Variables|Default|GetInteractSE) (Variables|Default|GetStaticMesh) "None" "0, 0, 0" "0, 0, 0" "KeepRelativeOffset" false 1.0 1.0 0.0 0 0)
  (Development|SetHiddeninGame (Variables|Default|GetStaticMesh) true false))

(event EventExitInspector
  (bind _bcanbestored (Variables|Default|GetbCanBeStored))
  (Audio|SpawnSoundAttached (Variables|Default|GetInteractSE) (Variables|Default|GetStaticMesh) "None" "0, 0, 0" "0, 0, 0" "KeepRelativeOffset" false 1.0 1.0 0.0 0 0)
  (Development|SetHiddeninGame (Variables|Default|GetStaticMesh) _bcanbestored false)
  (Collision|SetActorEnableCollision (not _bcanbestored)))

(fn ConstructionScript
  (|CallParentFunction))