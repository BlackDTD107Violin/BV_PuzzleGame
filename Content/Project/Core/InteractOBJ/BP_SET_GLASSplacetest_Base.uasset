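; BP_SET_GLASSplacetest_Base is an interactable placement spot that accepts a glass object of a matching type.
; On BeginPlay it caches the BP_FirstPersonCharacter player.
; On Interact it casts the passed actor to BP_CoreOBJ_GLASS and compares its GlassType with MatchGlassType.
; A match has the player assign the object to PlaceLocation and sets HavePlacedOBJ, while a wrong type or non-glass actor opens its own dialogue line.
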(event EventBeginPlay
  (|CallParentFunction)
  (bind _asbp_first_person_character (Utilities|Casting|CastToBP_FirstPersonCharacter (Game|GetPlayerCharacter 0)))
  (Variables|Default|SetPlayer _asbp_first_person_character))

(event EventInteract
  (params (InteractActor :type Actor%20Object%20Reference) (InteractTarget :type Actor%20Component%20Object%20Reference))
  (bind _asbp_core_obj_glass (Utilities|Casting|CastToBP_CoreOBJ_GLASS InteractActor)
    (:then
      (if (Utilities|Enum|Equal(Enum) (Variables|Default|GetMatchGlassType) (Variables|/Game/Project/Core/InteractOBJ/BP_CoreOBJ_GLASS.BP_CoreOBJ_GLASS_C|GetGlassType _asbp_core_obj_glass))
        (Default|OBJAssigntoSET (Variables|Default|GetPlayer) (Transformation|GetWorldLocation (Variables|Default|GetPlaceLocation)) self)
        (Variables|Default|SetbHavePlacedOBJ true)
        (else
          (Default|OpenDialogueTA (Variables|Default|GetPlayer) "800003"))))
    (:CastFailed
      (Default|OpenDialogueTA (Variables|Default|GetPlayer) "800002"))))

(fn ConstructionScript
  (|CallParentFunction))