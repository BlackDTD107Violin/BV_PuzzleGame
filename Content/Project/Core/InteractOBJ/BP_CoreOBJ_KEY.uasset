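; BP_CoreOBJ_KEY is the key variant of the core interactable object, tagging its object type on BeginPlay after parent setup.
; Entering the inspector marks the extract trigger area it was previously inserted in as empty and re-enables query and physics collision on that area's key trigger.
; ReturnKEYCode supplies the key's code and returns "None" here.
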(event EventBeginPlay
  (CallFunction|SetupParent)
  (Variables|Default|SetThisOBJtype "NewEnumerator1"))

(event EventEnterInspector
  (bind _currentinsertedextractta_old (Variables|Default|GetCurrentInsertedExtractTA_Old))
  (Variables|/Game/Project/InteractOBJ/BP_Extract_TA.BP_Extract_TA_C|SetbExtractTAIsEmpty _currentinsertedextractta_old true)
  (Collision|SetCollisionEnabled (Variables|/Game/Project/InteractOBJ/BP_Extract_TA.BP_Extract_TA_C|GetKey_TriggerArea _currentinsertedextractta_old) "QueryAndPhysics"))

(fn ConstructionScript
  (|CallParentFunction))

(fn ReturnKEYCode
  (return "None"))