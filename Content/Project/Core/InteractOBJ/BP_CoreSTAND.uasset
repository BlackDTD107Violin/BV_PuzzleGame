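; BP_CoreSTAND is an interactable stand with a zoom-in inspection view, apparently a base class given its many stub functions.
; It caches child BP_CoreITEM actors and the player, then enables click and mouse-over input.
; Zoom-in blends the view to the stand, locks move and look input, clears prompts and disables widget triggers.
; Zoom-out restores the player view and input, then re-enables the triggers after a delay.
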(event EventZoomin
  (params (ZoomComponent :type Actor%20Component%20Object%20Reference))
  (bind _returnvalue (Game|GetPlayerController 0))
  (if (> (Utilities|Array|Length (Variables|Default|GetZoomInPoint)) 1)
    (CallFunction|AssignZoomPos ZoomComponent))
  (Variables|Default|SetbIsStandByState false)
  (Game|Player|SetViewTargetwithBlend (Game|GetPlayerController 0) self 0.5 "VTBlend_Linear" 0.0 true)
  (Input|SetIgnoreMoveInput _returnvalue true)
  (Input|SetIgnoreLookInput _returnvalue true)
  (Default|ClearGamePromptUIView (Variables|Default|GetPlayer))
  (CallFunction|SwitchTACollisionProfile false))

(event EventZoomOut
  (bind _returnvalue (Game|GetPlayerController 0))
  (Game|Player|SetViewTargetwithBlend (Game|GetPlayerController 0) (Game|GetPlayerCharacter 0) 0.5 "VTBlend_Linear" 0.0 true)
  (Input|ResetIgnoreMoveInput _returnvalue)
  (Input|ResetIgnoreLookInput _returnvalue)
  (CallFunction|SwitchMeshCollisionProfile false)
  (Variables|Default|SetbIsStandByState true)
  (Utilities|FlowControl|Delay (Variables|Default|GetDelayTime))
  (CallFunction|SwitchTACollisionProfile true))

(event EventBeginPlay
  (bind _returnvalue (Game|GetPlayerController 0))
  (Utilities|FlowControl|Sequence
    (:then_0
      (for _array_element (Actor|GetAllChildActors true)
        (bind _asbp_core_item (Utilities|Casting|CastToBP_CoreITEM _array_element))
        (Utilities|Array|Add (Variables|Default|GetChildLists) _asbp_core_item)))
    (:then_1
      (bind _asbp_first_person_character (Utilities|Casting|CastToBP_FirstPersonCharacter (Game|GetPlayerCharacter 0)))
      (Variables|Default|SetPlayer _asbp_first_person_character)
      (Input|EnableInput _returnvalue)
      (Variables|/Script/Engine.PlayerController|SetbEnableClickEvents _returnvalue true)
      (Variables|/Script/Engine.PlayerController|SetbEnableMouseOverEvents _returnvalue true))))

(fn ConstructionScript
  (for _array_element (Actor|GetAllChildActors true)
    (bind _asbp_core_item (Utilities|Casting|CastToBP_CoreITEM _array_element))
    (Utilities|Array|Add (Variables|Default|GetChildLists) _asbp_core_item)))

(fn AssignZoomPos
  (params (ZoomInComp :type Object%20Object%20Reference))
  (return))

(fn CheckCanTakeItem
  (params (CurrentMesh :type Static%20Mesh%20Component%20Object%20Reference) (bOpenDirIsPositive :type Boolean) (CurrentValue :type Float%20%28double-precision%29) (BorderValue :type Float%20%28double-precision%29)))

(fn PresetItemMesh)

(fn PresetZoominGroup)

(fn ResetCanTakeItem)

(fn StopContinuedSE
  (params (TargetSE :type Audio%20Component%20Object%20Reference))
  (if (Utilities|IsValid TargetSE)
    (Audio|Components|Audio|Stop TargetSE)
    (Components|DestroyComponent TargetSE)))

(fn SwitchMeshCollisionProfile
  (params (bIsBlock :type Boolean)))

(fn SwitchTACollisionProfile
  (params (bIsLock :type Boolean))
  (if bIsLock
    (for _array_element (Variables|Default|GetWidgetTriggerGroup)
      (Collision|SetCollisionProfileName _array_element "StandByMode" true :!class /Script/Engine.PrimitiveComponent))
    (else
      (for _array_element_2 (Variables|Default|GetWidgetTriggerGroup)
        (Collision|SetCollisionProfileName _array_element_2 "NoCollision" true :!class /Script/Engine.PrimitiveComponent)))))

(fn RemoveCanTakeItem
  (params (RemoveTarget :type Integer) (RemoveTargetParam :type BP%20Core%20ITEM%20Object%20Reference)))