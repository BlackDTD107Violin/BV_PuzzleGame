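; Extractable item Blueprint that can be picked up into an inspector and inserted into an extract TA actor.
; Entering inspection plays an interact sound, hides the mesh, and picks the item out of any TA it occupies, resetting that TA's place offset.
; Exiting plays the sound again, then hides the whole actor and disables its collision.
; Extraction glow and data access are delegated to ACExtractComponent.
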(event EventItemExtractGlowing
  (params (bIsExtracting :type Boolean))
  (Default|ItemExtractGlowing (Variables|Default|GetAC_ExtractComponent) bIsExtracting))

(event EventEnterInspector
  (Audio|SpawnSoundAttached (Variables|Default|GetInteractSE) (Variables|Default|GetStaticMesh) "None" "0, 0, 0" "0, 0, 0" "KeepRelativeOffset" false 1.0 1.0 0.0 0 0)
  (Development|SetHiddeninGame (Variables|Default|GetStaticMesh) true false)
  (bind _currentinsertedextractta (Variables|Default|GetCurrentInsertedExtractTA)
    (:then
      (Default|PickOutITEM _currentinsertedextractta)
      (Default|ResetPlaceOffset _currentinsertedextractta))
    (:else)))

(event EventExitInspector
  (Audio|SpawnSoundAttached (Variables|Default|GetInteractSE) (Variables|Default|GetStaticMesh) "None" "0, 0, 0" "0, 0, 0" "KeepRelativeOffset" false 1.0 1.0 0.0 0 0)
  (Rendering|SetActorHiddenInGame true)
  (Collision|SetActorEnableCollision false))

(fn ConstructionScript
  (|CallParentFunction))

(fn GetExtractData
  (return (Variables|/Game/Project/Core/InteractOBJ/AC_ExtractComponent.AC_ExtractComponent_C|GetExtractData (Variables|Default|GetAC_ExtractComponent))))