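; BP_CoreOBJ_SET is an interact-object Blueprint that acts as a set point grouping BP_CoreOBJ actors and tracking whether an object is placed.
; On BeginPlay it sets its object type and gathers child actors that cast to BP_CoreOBJ into SETLists.
; OBJDetachFromSET clears the placed-object flag, and StopContinuedSE stops and destroys a given sound component.
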(event EventBeginPlay
  (Variables|Default|SetThisOBJtype "NewEnumerator0")
  (for _array_element (Actor|GetAllChildActors true)
    (bind _asbp_core_obj (Utilities|Casting|CastToBP_CoreOBJ _array_element))
    (Utilities|Array|Add (Variables|Default|GetSETLists) _asbp_core_obj)))

(fn ConstructionScript
  (|CallParentFunction))

(fn OBJDetachfromSET
  (Variables|Default|SetbHavePlacedOBJ false))

(fn StopContinuedSE
  (params (TargetSE :type Audio%20Component%20Object%20Reference))
  (if (Utilities|IsValid TargetSE)
    (Audio|Components|Audio|Stop TargetSE)
    (Components|DestroyComponent TargetSE)))