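; AC_ExtractComponent is an actor component that drives an extraction glow on an interactable item's materials.
; ItemExtractGlowing takes an extracting flag and steps a lerp alpha up toward one or down toward zero by world delta seconds on each call.
; Each change is pushed through SetExtractMatVal, which writes the LerpAlpha scalar parameter on every material in ExtractMatgroups.
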(event Custom|Item%20Extract%20Glowing
  (params (bIsExtracting :type Boolean))
  (if bIsExtracting
    (if (< (Variables|Default|GetExtractLerpAlpha) 1.0)
      (bind _output_get (Variables|Default|SetExtractLerpAlpha (+ (Variables|Default|GetExtractLerpAlpha) (Utilities|Time|GetWorldDeltaSeconds))))
      (CallFunction|SetExtractMatVal _output_get))
    (elif (> (Variables|Default|GetExtractLerpAlpha) 0.0)
      (bind _output_get_2 (Variables|Default|SetExtractLerpAlpha (- (Variables|Default|GetExtractLerpAlpha) (Utilities|Time|GetWorldDeltaSeconds))))
      (CallFunction|SetExtractMatVal _output_get_2))))

(fn SetExtractMatVal
  (params (LerpVal :type Float%20%28double-precision%29))
  (for _array_element (Variables|Default|GetExtractMatgroups)
    (Rendering|Material|SetScalarParameterValue _array_element "LerpAlpha" LerpVal :!class /Script/Engine.MaterialInstanceDynamic)))