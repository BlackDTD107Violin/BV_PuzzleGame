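; BP_GLASS_Element is an interactable glass object that registers itself with the HUD's glass collection UI when restored.
; On BeginPlay it caches BP_CoreHUD and fills its ThisGlass data with itself plus an example texture and type, as demo setup.
; GLASSrestore passes that data to the collection widget's AssignGlass.
; SetupGlass lets the glass data be replaced from outside.
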(event EventBeginPlay
  (|CallParentFunction)
  (bind _asbp_core_hud (Utilities|Casting|CastToBP_CoreHUD (HUD|GetHUD (Game|GetPlayerController 0))))
  (Variables|Default|SetREF_UI_CoreHUD _asbp_core_hud)
  ;[0.05098 0.05098 0.05098] Just For Demo
  (Variables|Default|SetThisGlass (Utilities|Struct|MakeST_GlassCollection self 0 (Variables|Default|GetExampleTexture) (Variables|Default|GetExampleGlassType) 0 0 0 0)))

(event EventGLASSrestore
  (Default|AssignGlass (Variables|/Game/Project/Core/Widget/BP_CoreHUD.BP_CoreHUD_C|GetREF_UI_GlassCollection (Variables|Default|GetREF_UI_CoreHUD)) (Variables|Default|GetThisGlass)))

(fn ConstructionScript
  (|CallParentFunction))

(fn SetupGlass
  (params (Result :type ST%20Glass%20Collection%20Structure))
  (Variables|Default|SetThisGlass Result))