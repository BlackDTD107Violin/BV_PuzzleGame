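; BP_GlassRender_Unite is a render rig that shows a group of glass values on glass totem previewer child actors beside a scene capture.
; On BeginPlay it gathers eight BP_GlassTotemPreviewer child actors into RenderGroup and stores the SceneCaptureComponent2D's render target reference.
; UpdateRenderer passes each incoming glass value to the previewer at the same index, always using one fixed value side.
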(event EventBeginPlay
  (CallFunction|PresetValue))

(fn ConstructionScript)

(fn PresetValue
  (Utilities|FlowControl|Sequence
    (:then_0
      (bind _asbp_glass_totem_previewer (Utilities|Casting|CastToBP_GlassTotemPreviewer (Variables|/Script/Engine.ChildActorComponent|GetChildActor (Variables|Default|GetCA_GlassPreview))))
      (Utilities|Array|Add (Variables|Default|GetRenderGroup) _asbp_glass_totem_previewer)
      (bind _asbp_glass_totem_previewer_2 (Utilities|Casting|CastToBP_GlassTotemPreviewer (Variables|/Script/Engine.ChildActorComponent|GetChildActor (Variables|Default|GetCA_GlassPreview1))))
      (Utilities|Array|Add (Variables|Default|GetRenderGroup) _asbp_glass_totem_previewer_2))
    (:then_1
      (bind _asbp_glass_totem_previewer_3 (Utilities|Casting|CastToBP_GlassTotemPreviewer (Variables|/Script/Engine.ChildActorComponent|GetChildActor (Variables|Default|GetCA_GlassPreview2))))
      (Utilities|Array|Add (Variables|Default|GetRenderGroup) _asbp_glass_totem_previewer_3)
      (bind _asbp_glass_totem_previewer_4 (Utilities|Casting|CastToBP_GlassTotemPreviewer (Variables|/Script/Engine.ChildActorComponent|GetChildActor (Variables|Default|GetCA_GlassPreview3))))
      (Utilities|Array|Add (Variables|Default|GetRenderGroup) _asbp_glass_totem_previewer_4))
    (:then_2
      (bind _asbp_glass_totem_previewer_5 (Utilities|Casting|CastToBP_GlassTotemPreviewer (Variables|/Script/Engine.ChildActorComponent|GetChildActor (Variables|Default|GetCA_GlassPreview4))))
      (Utilities|Array|Add (Variables|Default|GetRenderGroup) _asbp_glass_totem_previewer_5)
      (bind _asbp_glass_totem_previewer_6 (Utilities|Casting|CastToBP_GlassTotemPreviewer (Variables|/Script/Engine.ChildActorComponent|GetChildActor (Variables|Default|GetCA_GlassPreview5))))
      (Utilities|Array|Add (Variables|Default|GetRenderGroup) _asbp_glass_totem_previewer_6))
    (:then_3
      (bind _asbp_glass_totem_previewer_7 (Utilities|Casting|CastToBP_GlassTotemPreviewer (Variables|/Script/Engine.ChildActorComponent|GetChildActor (Variables|Default|GetCA_GlassPreview6))))
      (Utilities|Array|Add (Variables|Default|GetRenderGroup) _asbp_glass_totem_previewer_7)
      (bind _asbp_glass_totem_previewer_8 (Utilities|Casting|CastToBP_GlassTotemPreviewer (Variables|/Script/Engine.ChildActorComponent|GetChildActor (Variables|Default|GetCA_GlassPreview7))))
      (Utilities|Array|Add (Variables|Default|GetRenderGroup) _asbp_glass_totem_previewer_8))
    (:then_4
      (Variables|Default|SetREF_Texture%20Target (Variables|/Script/Engine.SceneCaptureComponent2D|GetTextureTarget (Variables|Default|GetSceneCaptureComponent2D))))))

(fn UpdateRenderer
  (params (GlassValueGroup :type Array%20of%20ST%20Glass%20Value%20Structures))
  (bind _output_get (LocalVariables|SetL_GlassValueGroup GlassValueGroup))
  (bind _output_get_2 (LocalVariables|SetL_GlassValueCount_Total (Utilities|Array|Length _output_get)))
  (bind _index (Utilities|FlowControl|ForLoopwithBreak 0 (- _output_get_2 1))
    (:LoopBody
      (Default|ReceiveGLASSPreviewer :self (Utilities|Array|Get(acopy) (Variables|Default|GetRenderGroup) _index) :ValueSide "NewEnumerator3" :CurrentGlassValue (Utilities|Array|Get(acopy) (LocalVariables|GetL_GlassValueGroup) _index)))))