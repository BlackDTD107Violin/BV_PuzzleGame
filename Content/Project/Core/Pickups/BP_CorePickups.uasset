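; BP_CorePickups is a core pickup Blueprint that provides shared setup functions for pickup actors.
; SetupParent stores the original transform and flags whether the actor has a valid parent actor.
; SetupWidget creates pick and interact prompt widgets, adds both to the viewport hidden, and keeps references to them.
; ReturnOBJCode returns a placeholder key serial and extract code, indicating no key by default.
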(fn ConstructionScript)

(fn SetupParent
  (Variables|Default|SetOriginalPos (Transformation|GetActorTransform))
  (Utilities|IsValid (Actor|GetParentActor)
    (:Is%20Valid
      (Variables|Default|SetbHasParent true))))

(fn SetupWidget
  (bind _returnvalue (UserInterface|CreateWidget "/Game/Project/Widget/WBP_PickPrompt.WBP_PickPrompt_C"))
  (bind _output_get (Variables|Default|SetREF_PickPrompt _returnvalue))
  (UserInterface|Viewport|AddtoViewport _output_get 1)
  (Widget|SetVisibility (Variables|Default|GetREF_PickPrompt) "Hidden")
  (bind _returnvalue_2 (UserInterface|CreateWidget "/Game/Project/Widget/WBP_InteractPrompt.WBP_InteractPrompt_C"))
  (bind _output_get_2 (Variables|Default|SetREF_InteractPrompt _returnvalue_2))
  (UserInterface|Viewport|AddtoViewport _output_get_2 1)
  (Widget|SetVisibility (Variables|Default|GetREF_InteractPrompt) "Hidden"))

(fn ReturnOBJCode
  (return "None" 0))