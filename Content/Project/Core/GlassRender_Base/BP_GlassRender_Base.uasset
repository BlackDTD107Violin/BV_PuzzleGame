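; BP_GlassRender_Base is a render rig that previews a glass totem through a SceneCaptureComponent2D and a BP_GlassTotemPreviewer child actor.
; On BeginPlay it caches the capture's texture target and the previewer cast from that child actor.
; UpdateRenderer passes a glass value to the previewer's ReceiveGLASSPreviewer with a fixed side enum.
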(event EventBeginPlay
  (CallFunction|PresetValue))

(fn ConstructionScript)

(fn PresetValue
  (Utilities|FlowControl|Sequence
    (:then_0
      (Variables|Default|SetREF_Texture%20Target (Variables|/Script/Engine.SceneCaptureComponent2D|GetTextureTarget (Variables|Default|GetSceneCaptureComponent2D))))
    (:then_1
      (bind _asbp_glass_totem_previewer (Utilities|Casting|CastToBP_GlassTotemPreviewer (Variables|/Script/Engine.ChildActorComponent|GetChildActor (Variables|Default|GetCA_GlassPreview))))
      (Variables|Default|SetREF_Previewer _asbp_glass_totem_previewer))))

(fn UpdateRenderer
  (params (GlassValue :type ST%20Glass%20Value%20Structure))
  (Default|ReceiveGLASSPreviewer :self (Variables|Default|GetREF_Previewer) :ValueSide "NewEnumerator5" :CurrentGlassValue GlassValue))