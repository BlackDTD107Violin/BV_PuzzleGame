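; BP_Studio_DD is an inspection studio actor that displays a given item's mesh for viewing.
; AssignInspectorData stores the mesh, initial rotation and scale, then SetupInspectorData applies them to the ItemToFocus component.
; Logic to hand input from the first-person or tutorial character to the studio is present but disconnected.
; AttachtoHand and the code and list getters are empty stubs returning defaults.
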(event EventAssignInspectorData
  (params (ItemToFocus :type Static%20Mesh%20Object%20Reference) (InitRotation :type Rotator :default "0, 0, 0") (InitScale :type Vector :default "0, 0, 0") (FirstPerson :type BP%20First%20Person%20Character%20Object%20Reference) (FirstPersonTutorial :type BP%20First%20Person%20Character%20Tutorial%20Object%20Reference))
  (Variables|Default|SetItem%20to%20Focus ItemToFocus)
  (Variables|Default|SetInit%20Rotation InitRotation)
  (Variables|Default|SetInit%20Scale InitScale)
  (CallFunction|SetupInspectorData))

(fn ConstructionScript)

(fn SetupInspectorData
  (Components|StaticMesh|SetStaticMesh (Variables|Default|GetItemToFocus) (Variables|Default|GetItem%20to%20Focus))
  (Transformation|SetRelativeRotation (Variables|Default|GetItemToFocus) (Variables|Default|GetInit%20Rotation) false false)
  (Transformation|SetRelativeScale3D (Variables|Default|GetItemToFocus) (Variables|Default|GetInit%20Scale)))

(fn AttachtoHand
  (params (InteractTarget :type Actor%20Component%20Object%20Reference))
  (return 0))

(fn ReturnExtractCode
  (return 0))

(fn ReturnOBJCode
  (return "None"))

(fn ReturnTRICKLists
  (return 0))