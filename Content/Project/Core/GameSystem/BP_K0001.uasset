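; BP_K0001 is an actor, apparently a key object, that can return to its original placement.
; Repos restores the stored relative transform and, if HasParent is set, snaps a component onto the ReAttach component at the socket named by KeySerialCode.
; SetTempPos supplies that reattach target, while BeginPlay and the construction script only call their parents.
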(event EventBeginPlay
  (|CallParentFunction))

(event EventSetTempPos
  (params (Root :type Static%20Mesh%20Component%20Object%20Reference))
  (Variables|Default|SetReattach Root))

(event EventRepos
  (Transformation|SetActorRelativeTransform (Variables|Default|GetOriginalPos) false false)
  (if (Variables|Default|GetbHasParent)
    (Transformation|AttachComponentToComponent (Variables|Default|GetReAttach) (Variables|Default|GetKeySerialCode) "SnapToTarget" "SnapToTarget" "SnapToTarget" true)))

(fn ConstructionScript
  (|CallParentFunction))