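; Manager actor for the player hint system, offering up to three timed hints per checkpoint.
; Tick timers unlock hints; holding H fills a bar that opens the hint panel and toggles player control.
; Hint text comes from DT_GameHintTable rows indexed by checkpoint and hint, localized through the stage manager's language code.
; It binds to two film actors' start/end events and has pause/resume handlers for the timer.
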(event Custom|PauseTimer
  (Actor|Tick|SetActorTickEnabled false)
  (Variables|Default|SetKeyHPercentage 0.0)
  (if (> (Variables|Default|GetTotalHint) 0)
    (Default|CloseHintKeyH (Variables|Default|GetREF_CoreHUD))))

(event Custom|ResumeTimer
  (Actor|Tick|SetActorTickEnabled true)
  (if (> (Variables|Default|GetTotalHint) 0)
    (Default|OpenHintKeyH (Variables|Default|GetREF_CoreHUD))))

(event Custom|RefreshLanguage
  (bind _returnvalue (Utilities|GetDataTableRow "/Game/Project/DataTable/DT_GameHintTable.DT_GameHintTable" (Variables|Default|GetCurrentRowName))
    (:then
      (bind _content (CallFunction|GetMatchLanguage _returnvalue))
      (Default|UpdateGameHint (Variables|Default|GetREF_CoreHUD) _content true))))

(event Custom|SwitchDynamicTextLanguage
  (Variables|Default|SetLanguageCode (Variables|/Game/Project/Core/GameSystem/BP_StageManager.BP_StageManager_C|GetLanguageCode (Variables|Default|GetREF_StageManager)))
  (CallFunction|RefreshLanguage))

(event EventBeginPlay
  (bind _asbp_core_hud (Utilities|GetCoreHUDinTime 1e+01)
    (:Success
      (Variables|Default|SetREF_CoreHUD _asbp_core_hud)
      (Utilities|FlowControl|DelayUntilNextTick)
      (EventDispatchers|BindEventtoSwitchLanguageCode (Variables|Default|GetREF_StageManager) (EventDispatchers|CreateEvent :!event Custom|SwitchDynamicTextLanguage))
      (CallFunction|UpdateFirstHint)
      (bind _asbp_first_person_character (Utilities|Casting|CastToBP_FirstPersonCharacter (Game|GetPlayerCharacter 0)))
      (Variables|Default|SetREF_Player _asbp_first_person_character)
      (CallFunction|GetAllFilmREFS)
      (Actor|Tick|SetActorTickEnabled true))))

(event EventTick
  (params (DeltaSeconds :type Float%20%28single-precision%29))
  (Utilities|FlowControl|Sequence
    (:then_0
      (if (and (Variables|Default|GetbIsPressingH) (Variables|Default|GetbCanHint))
        (CallFunction|KeyHBarLoading)))
    (:then_1
      (if (and (== (Variables|Default|GetTotalHint) 0) (not (Variables|Default|GetbFirstHintActivate)))
        (CallFunction|HintTimerTickingFirst)
        (elif (and (<= (Variables|Default|GetTotalHint) 2) (Variables|Default|GetbFirstHintActivate))
          (CallFunction|HintTimerTickingOther))))))

(fn ConstructionScript)

(fn AcquireHintContent
  (bind _output_get (Variables|Default|SetCurrentRowName (Utilities|String|StringToName (Utilities|String|ToString(Integer) (+ (* (Variables|Default|GetCheckPoint) 3) (+ (Variables|Default|GetCurrentHint) 1))))))
  (bind _returnvalue (Utilities|GetDataTableRow "/Game/Project/DataTable/DT_GameHintTable.DT_GameHintTable" _output_get)
    (:then
      (bind _content (CallFunction|GetMatchLanguage _returnvalue))
      (Default|UpdateGameHint (Variables|Default|GetREF_CoreHUD) _content false))))

(fn HintTimerTickingFirst
  (bind _output_get (Variables|Default|SetHintTimer (+ (Utilities|Time|GetWorldDeltaSeconds) (Variables|Default|GetHintTimer))))
  (if (>= _output_get (Variables|Default|GetFirstHintEnableLimit))
    (Default|OpenHintKeyH (Variables|Default|GetREF_CoreHUD))
    (Variables|Default|SetbCanHint true)
    (Default|UpdateHintTimer (Variables|Default|GetREF_CoreHUD) (Variables|Default|GetTotalHint) 1.0)
    (Variables|Default|SetHintTimer 0.0)
    (bind _result (Math|Integer|IncrementInt (Variables|Default|GetTotalHint))
      (:%20%20
        (Default|SetupNewHintCounter (Variables|Default|GetREF_CoreHUD) _result)))))

(fn HintTimerTickingOther
  (bind _output_get (Variables|Default|SetHintTimer (+ (Utilities|Time|GetWorldDeltaSeconds) (Variables|Default|GetHintTimer))))
  (if (>= _output_get (Variables|Default|GetOtherHintEnableLimit))
    (Default|UpdateHintTimer (Variables|Default|GetREF_CoreHUD) (Variables|Default|GetTotalHint) 1.0)
    (Variables|Default|SetHintTimer 0.0)
    (Utilities|Array|SetArrayElem (Variables|Default|GetHintState) (Variables|Default|GetTotalHint) "NewEnumerator2")
    (bind _result (Math|Integer|IncrementInt (Variables|Default|GetTotalHint))
      (:%20%20
        (Default|SetupNewHintCounter (Variables|Default|GetREF_CoreHUD) _result)))
    (else
      (Default|UpdateHintTimer (Variables|Default|GetREF_CoreHUD) (Variables|Default|GetTotalHint) (/ (Variables|Default|GetHintTimer) (Variables|Default|GetOtherHintEnableLimit))))))

(fn KeyHBarLoading
  (bind _ref_player (Variables|Default|GetREF_Player))
  (Utilities|FlowControl|Sequence
    (:then_0
      (bind _output_get (Variables|Default|SetKeyHPercentage (+ (Variables|Default|GetKeyHPercentage) (Utilities|Time|GetWorldDeltaSeconds))))
      (Default|UpdateKeyHBar (Variables|Default|GetREF_CoreHUD) _output_get))
    (:then_1
      (if (>= (Variables|Default|GetKeyHPercentage) 1.0)
        (bind _output_get_2 (Variables|Default|SetKeyHPercentage 0.0))
        (Default|UpdateKeyHBar (Variables|Default|GetREF_CoreHUD) _output_get_2)
        (Variables|Default|SetbIsPressingH false)
        (Variables|Default|SetbCanHint false)
        (Variables|/Game/ProjectDefault/FirstPerson/Blueprints/BP_FirstPersonCharacter.BP_FirstPersonCharacter_C|SetbCoverByGameHint _ref_player true)
        (Default|TogglePlayerCtrl _ref_player true)
        (Default|OpenGameHint (Variables|Default|GetREF_CoreHUD))
        (CallFunction|AcquireHintContent)
        (if (not (Variables|Default|GetbFirstHintActivate))
          (Variables|Default|SetbFirstHintActivate true))))))

(fn ResetHintProgress
  (Variables|Default|SetHintTimer 0.0)
  (Variables|Default|SetTotalHint 0)
  (Variables|Default|SetCheckPoint 0))

(fn ResetKeyHProgress
  (Variables|Default|SetbIsPressingH false)
  (bind _output_get (Variables|Default|SetKeyHPercentage 0.0))
  (Default|UpdateKeyHBar (Variables|Default|GetREF_CoreHUD) _output_get))

(fn RequestSwitchHint
  (LocalVariables|SetL_OriginalHint (Variables|Default|GetCurrentHint))
  (Utilities|FlowControl|ForLoopwithBreak 0 2 :!label _label
    (:LoopBody
      (bind _result (Math|Integer|IncrementInt (Variables|Default|GetCurrentHint))
        (:%20%20
          (if (> _result 2)
            (Variables|Default|SetCurrentHint 0))
          (if (Utilities|Enum|Equal(Enum) (Utilities|Array|Get(acopy) (Variables|Default|GetHintState) (Variables|Default|GetCurrentHint)) "NewEnumerator2")
            (goto _label Break)))))
    (:Completed
      (if (!= (LocalVariables|GetL_OriginalHint) (Variables|Default|GetCurrentHint))
        (Utilities|Array|SetArrayElem (Variables|Default|GetHintState) (LocalVariables|GetL_OriginalHint) "NewEnumerator2")
        (Utilities|Array|SetArrayElem (Variables|Default|GetHintState) (Variables|Default|GetCurrentHint) "NewEnumerator1")
        (CallFunction|AcquireHintContent)
        (Default|SwitchHintCounter (Variables|Default|GetREF_CoreHUD) (Variables|Default|GetCurrentHint))))))

(fn UpdateFirstHint
  (bind _output_get (Variables|Default|SetCurrentRowName (Utilities|String|StringToName (Utilities|String|ToString(Integer) (+ (* (Variables|Default|GetCheckPoint) 3) 1)))))
  (bind _returnvalue (Utilities|GetDataTableRow "/Game/Project/DataTable/DT_GameHintTable.DT_GameHintTable" _output_get)
    (:then
      (bind _content (CallFunction|GetMatchLanguage _returnvalue))
      (Default|UpdateGameHint (Variables|Default|GetREF_CoreHUD) _content true)
      (Default|SwitchHintCounter (Variables|Default|GetREF_CoreHUD)))))

(fn UpdateCheckPoint
  (bind _ref_corehud (Variables|Default|GetREF_CoreHUD))
  (bind _hintstate (Variables|Default|GetHintState))
  (bind _result (Math|Integer|IncrementInt (Variables|Default|GetCheckPoint))
    (:%20%20
      (if (<= (Variables|Default|GetMaxCheckPoint) _result)
        (CallFunction|UpdateFirstHint))
      (Utilities|FlowControl|Sequence
        (:then_0
          (Utilities|Array|SetArrayElem _hintstate 1 "NewEnumerator0")
          (Utilities|Array|SetArrayElem _hintstate 2 "NewEnumerator0")
          (Default|CloseHintKeyH _ref_corehud)
          (Default|ResetHintCounter _ref_corehud))
        (:then_1
          (Variables|Default|SetTotalHint 0)
          (Variables|Default|SetCurrentHint 0)
          (Variables|Default|SetHintTimer 0.0)
          (Variables|Default|SetbFirstHintActivate false)
          (Variables|Default|SetbCanHint false))))))

(fn GetAllFilmREFS
  (Utilities|FlowControl|Sequence
    (:then_0
      (bind _returnvalue (Actor|GetActorOfClass "/Game/Project/InteractOBJ/BP_S9008.BP_S9008_C"))
      (Variables|Default|SetREF_S9008 _returnvalue)
      (bind _returnvalue_2 (Actor|GetActorOfClass "/Game/Project/InteractOBJ/BP_S9009.BP_S9009_C"))
      (Variables|Default|SetREF_S9009 _returnvalue_2))
    (:then_1
      (EventDispatchers|BindEventtoFilmStart (Variables|Default|GetREF_S9008) (EventDispatchers|CreateEvent :!event Custom|PauseTimer))
      (EventDispatchers|BindEventtoFilmStart (Variables|Default|GetREF_S9009) (EventDispatchers|CreateEvent :!event Custom|PauseTimer)))
    (:then_2
      (EventDispatchers|BindEventtoFilmEnd (Variables|Default|GetREF_S9008) (EventDispatchers|CreateEvent :!event Custom|ResumeTimer))
      (EventDispatchers|BindEventtoFilmEnd (Variables|Default|GetREF_S9009) (EventDispatchers|CreateEvent :!event Custom|ResumeTimer)))))

(fn GetMatchLanguage
  (params (OutRow :type F%20Game%20Hint%20Struct%20Structure))
  (bind (_content_zh_tw _content_en _content_ja) (Utilities|Struct|BreakF_GameHintStruct OutRow))
  (switch int (Variables|Default|GetLanguageCode)
    (:0
      (return _content_zh_tw))
    (:1
      (return _content_en))
    (:2
      (return _content_ja))))