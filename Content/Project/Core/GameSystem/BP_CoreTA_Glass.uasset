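; Glass slot trigger area on the mixer/calculate, extract and certify machines (BP_S9001, BP_S9008, BP_S9009), holding one glass item.
; GlassTAside selects the parent machine, which receives inserted glass data and tracks the attached item.
; Extract and mix results pull glass from the manager's pool, fill its data and disable trigger collision until pickup.
; Placed glass gets its mesh by type and a per-side render-target totem material.
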(event EventBeginPlay
  (|CallParentFunction)
  (switch Utilities|FlowControl|Switch|SwitchonE_GlassSideState (Variables|Default|GetGlassTAside)
    (:NewEnumerator1
      (bind _asbp_s9001 (Utilities|Casting|CastToBP_S9001 (Variables|Default|GetParentActor) :!label _label))
      (Variables|Default|SetREF_MainMachine _asbp_s9001))
    (:NewEnumerator2
      (goto _label))
    (:NewEnumerator3
      (goto _label))
    (:NewEnumerator4
      (goto _label))
    (:NewEnumerator5
      (bind _asbp_s9008 (Utilities|Casting|CastToBP_S9008 (Variables|Default|GetParentActor)))
      (Variables|Default|SetREF_ExtractMachine _asbp_s9008))
    (:NewEnumerator6
      (bind _asbp_s9009 (Utilities|Casting|CastToBP_S9009 (Variables|Default|GetParentActor)))
      (Variables|Default|SetREF_CertifyMachine _asbp_s9009))))

(fn ConstructionScript
  (|CallParentFunction))

(fn ReceiveExtractDataandCreate
  (params (GlassBase :type ST%20Glass%20Value%20Structure))
  (LocalVariables|SetL_CurrentExtractData GlassBase)
  (Utilities|FlowControl|Sequence
    (:then_0
      (bind _glassfrompool (Default|AcquireGlassfromPool (Variables|Default|GetREF_GlassManager)))
      (bind _output_get (LocalVariables|SetL_Temp_GLASSbase _glassfrompool))
      (Transformation|SetActorTransform _output_get (Math|Conversions|ToTransform(Vector) (Transformation|GetWorldLocation (Variables|Default|GetPlaceLocation))))
      (Variables|/Game/Project/InteractOBJ/BP_GLASSItem.BP_GLASSItem_C|SetThisGlass (LocalVariables|GetL_Temp_GLASSbase) (Utilities|Struct|MakeST_GlassData (LocalVariables|GetL_Temp_GLASSbase) -1 0 (Utilities|Array|MakeArray (LocalVariables|GetL_CurrentExtractData)) 0 0))
      (bind _previewmat (Default|ReturnRenderMatScene (Variables|/Game/Project/InteractOBJ/BP_GLASSItem.BP_GLASSItem_C|GetREF_GlassManager (LocalVariables|GetL_Temp_GLASSbase))))
      (Rendering|Material|SetMaterial (Variables|/Game/Project/Core/InteractOBJ/BP_CoreOBJ.BP_CoreOBJ_C|GetStaticMesh (LocalVariables|GetL_Temp_GLASSbase)) 3 _previewmat)
      (Default|SwitchStateRenderMatScene (Variables|/Game/Project/InteractOBJ/BP_GLASSItem.BP_GLASSItem_C|GetREF_GlassManager (LocalVariables|GetL_Temp_GLASSbase)) 0 true))
    (:then_1
      (CallFunction|SetupNewGlassItem (LocalVariables|GetL_Temp_GLASSbase))
      (Collision|SetCollisionEnabled (Variables|Default|GetMain_TriggerArea) "NoCollision")
      (Collision|SetCollisionEnabled (Variables|/Game/Project/Core/InteractOBJ/BP_CoreOBJ.BP_CoreOBJ_C|GetStaticMesh (Variables|Default|GetREF_InsertedGLASS)) "NoCollision"))))

(fn ReceiveMixDataandCreate
  (params (GlassUnite :type ST%20Glass%20Data%20Structure))
  (Variables|Default|SetInsertedGlassData GlassUnite)
  (Utilities|FlowControl|Sequence
    (:then_0
      (bind _glassfrompool (Default|AcquireGlassfromPool (Variables|Default|GetREF_GlassManager)))
      (bind _output_get (LocalVariables|SetL_Temp_GLASSbase _glassfrompool))
      (Transformation|SetActorTransform _output_get (Math|Conversions|ToTransform(Vector) (Transformation|GetWorldLocation (Variables|Default|GetPlaceLocation))))
      (Variables|/Game/Project/InteractOBJ/BP_GLASSItem.BP_GLASSItem_C|SetThisGlass (LocalVariables|GetL_Temp_GLASSbase) (Utilities|Struct|MakeST_GlassData (LocalVariables|GetL_Temp_GLASSbase) -1 (.inheritlayer (Variables|Default|GetInsertedGlassData)) (.glassvalue (Variables|Default|GetInsertedGlassData)) 0 0))
      (Variables|/Game/Project/Core/InteractOBJ/BP_CoreITEM_GLASS.BP_CoreITEM_GLASS_C|SetGlassType (LocalVariables|GetL_Temp_GLASSbase) "NewEnumerator1")
      (switch int (.inheritlayer (Variables|Default|GetInsertedGlassData))
        (:1
          (Variables|/Game/Project/Core/InteractOBJ/BP_CoreOBJ.BP_CoreOBJ_C|SetOBJSerialCode (LocalVariables|GetL_Temp_GLASSbase) "G_Unite1"))
        (:2
          (Variables|/Game/Project/Core/InteractOBJ/BP_CoreOBJ.BP_CoreOBJ_C|SetOBJSerialCode (LocalVariables|GetL_Temp_GLASSbase) "G_Unite2"))
        (:3
          (Variables|/Game/Project/Core/InteractOBJ/BP_CoreOBJ.BP_CoreOBJ_C|SetOBJSerialCode (LocalVariables|GetL_Temp_GLASSbase) "G_Unite3"))))
    (:then_1
      (CallFunction|SetupNewGlassItem (LocalVariables|GetL_Temp_GLASSbase) 4)
      (Collision|SetCollisionEnabled (Variables|Default|GetMain_TriggerArea) "NoCollision")
      (Collision|SetCollisionEnabled (Variables|/Game/Project/Core/InteractOBJ/BP_CoreOBJ.BP_CoreOBJ_C|GetStaticMesh (Variables|Default|GetREF_InsertedGLASS)) "NoCollision"))))

(fn RefreshInsertedDataGlass
  (params (Glass%20Data :type ST%20Glass%20Data%20Structure))
  (bind _ref_certifymachine (Variables|Default|GetREF_CertifyMachine))
  (Variables|Default|SetInsertedGlassData Glass%20Data)
  (Utilities|FlowControl|Sequence
    (:then_0
      (LocalVariables|SetL_GlassValues (Utilities|Struct|BreakST_GlassData (Variables|Default|GetInsertedGlassData)))
      (Audio|SpawnSoundAttached "/Game/Project/Audio/MetaSoundSource/SE/MSS_Pick_Place_Metal_5.MSS_Pick_Place_Metal_5" (Variables|Default|GetPlaceLocation) "None" "0, 0, 0" "0, 0, 0" "KeepRelativeOffset" false 1.0 1.0 0.0 0 0))
    (:then_1
      (switch Utilities|FlowControl|Switch|SwitchonE_GlassSideState (Variables|Default|GetGlassTAside)
        (:NewEnumerator1
          (Variables|/Game/Project/InteractOBJ/BP_S9001.BP_S9001_C|SetLeftInsertedGlass (Variables|Default|GetREF_MainMachine) (Variables|Default|GetInsertedGlassData))
          (Variables|Default|SetSideIndex 2))
        (:NewEnumerator2
          (Variables|/Game/Project/InteractOBJ/BP_S9001.BP_S9001_C|SetRightInsertedGlass (Variables|Default|GetREF_MainMachine) (Variables|Default|GetInsertedGlassData))
          (Variables|Default|SetSideIndex 3))
        (:NewEnumerator4
          (Variables|/Game/Project/InteractOBJ/BP_S9001.BP_S9001_C|SetDownInsertedGlass (Variables|Default|GetREF_MainMachine) (Variables|Default|GetInsertedGlassData))
          (Variables|Default|SetSideIndex 1)
          (Variables|/Game/Project/InteractOBJ/BP_S9001.BP_S9001_C|SetDownInsertedGlassValue (Variables|Default|GetREF_MainMachine) (Utilities|Array|Get(acopy) (LocalVariables|GetL_GlassValues))))
        (:NewEnumerator6
          (Variables|/Game/Project/InteractOBJ/BP_S9009.BP_S9009_C|SetInsertedGlass _ref_certifymachine (Variables|Default|GetInsertedGlassData))
          (Variables|Default|SetSideIndex 4)
          (Default|CertifyStartCheckMatchCode _ref_certifymachine)))
      (CallFunction|SpawnGLASS (Variables|Default|GetSideIndex) (Utilities|Struct|BreakST_GlassData (Variables|Default|GetInsertedGlassData)))
      (Variables|/Game/Project/Core/InteractOBJ/BP_CoreITEM_GLASS.BP_CoreITEM_GLASS_C|SetCurrentInsertedTA (Utilities|Struct|BreakST_GlassData (Variables|Default|GetInsertedGlassData)) self)
      (Rendering|SetActorHiddenInGame (Utilities|Struct|BreakST_GlassData (Variables|Default|GetInsertedGlassData)) false)
      (Collision|SetActorEnableCollision (Utilities|Struct|BreakST_GlassData (Variables|Default|GetInsertedGlassData)) true)
      (Variables|Default|SetbThisTAIsEmpty false))))

(fn ResetAfterMerge
  (Variables|Default|SetbThisTAIsEmpty true)
  (Collision|SetCollisionEnabled (Variables|Default|GetMain_TriggerArea) "QueryAndPhysics"))

(fn PickOutGLASS
  (bind _ref_extractmachine (Variables|Default|GetREF_ExtractMachine))
  (Utilities|FlowControl|Sequence
    (:then_0
      (Variables|Default|SetbThisTAIsEmpty true)
      (Collision|SetCollisionEnabled (Variables|Default|GetMain_TriggerArea) "QueryAndPhysics")
      (Variables|/Game/Project/Core/InteractOBJ/BP_CoreITEM.BP_CoreITEM_C|SetbCanTake (Variables|Default|GetREF_InsertedGLASS) false)
      (switch Utilities|FlowControl|Switch|SwitchonE_GlassSideState (Variables|Default|GetGlassTAside)
        (:NewEnumerator1
          (Utilities|Array|RemoveItem (Variables|/Game/Project/Core/InteractOBJ/BP_CoreSTAND.BP_CoreSTAND_C|GetChildLists (Variables|Default|GetREF_MainMachine)) (Variables|Default|GetREF_InsertedGLASS) :!label _label))
        (:NewEnumerator2
          (goto _label))
        (:NewEnumerator3
          (goto _label))
        (:NewEnumerator4
          (goto _label))
        (:NewEnumerator5
          (Utilities|Array|RemoveItem (Variables|/Game/Project/Core/InteractOBJ/BP_CoreSTAND.BP_CoreSTAND_C|GetChildLists (Variables|Default|GetREF_ExtractMachine)) (Variables|Default|GetREF_InsertedGLASS)))
        (:NewEnumerator6
          (Utilities|Array|RemoveItem (Variables|/Game/Project/Core/InteractOBJ/BP_CoreSTAND.BP_CoreSTAND_C|GetChildLists (Variables|Default|GetREF_CertifyMachine)) (Variables|Default|GetREF_InsertedGLASS)))))
    (:then_1
      (Utilities|IsValid (Variables|Default|GetREF_ExtractMachine)
        (:Is%20Valid
          (Variables|/Game/Project/InteractOBJ/BP_S9008.BP_S9008_C|SetbResultIsEmpty _ref_extractmachine true)
          (Default|CheckState-DiamondCurrent _ref_extractmachine))
        (:Is%20Not%20Valid
          _))
      (return (Variables|Default|GetGlassTAside)))))

(fn RemoveGlassTAside
  (params (Side :type E_GlassSideState%20Enum :default "NewEnumerator0"))
  (Default|EraseTotemPreviewer (Variables|Default|GetREF_MainMachine) Side))

(fn SetupNewGlassItem
  (params (Glass%20Data :type BP%20Core%20ITEM%20GLASS%20Object%20Reference) (SideIndex :type Integer))
  (LocalVariables|SetL_GlassData Glass%20Data)
  (CallFunction|SpawnGLASS SideIndex (LocalVariables|GetL_GlassData))
  (Variables|/Game/Project/Core/InteractOBJ/BP_CoreITEM_GLASS.BP_CoreITEM_GLASS_C|SetCurrentInsertedTA (LocalVariables|GetL_GlassData) self)
  (Rendering|SetActorHiddenInGame (LocalVariables|GetL_GlassData) false)
  (Collision|SetActorEnableCollision (LocalVariables|GetL_GlassData) true))

(fn SpawnGLASS
  (params (SideIndex :type Integer) (GlassData :type BP%20Core%20ITEM%20GLASS%20Object%20Reference))
  (LocalVariables|SetL_SideIndex SideIndex)
  (bind _asbp_glassitem (Utilities|Casting|CastToBP_GLASSItem GlassData))
  (bind _output_get (Variables|Default|SetREF_InsertedGLASS _asbp_glassitem))
  (Variables|/Game/Project/Core/InteractOBJ/BP_CoreITEM.BP_CoreITEM_C|SetbCanTake _output_get true)
  (Utilities|FlowControl|Sequence
    (:then_0
      (LocalVariables|SetL_GlassValue (.glassvalue (Variables|/Game/Project/InteractOBJ/BP_GLASSItem.BP_GLASSItem_C|GetThisGlass (Variables|Default|GetREF_InsertedGLASS))))
      (if (Utilities|Enum|Equal(Enum) (Variables|/Game/Project/Core/InteractOBJ/BP_CoreITEM_GLASS.BP_CoreITEM_GLASS_C|GetGlassType (Variables|Default|GetREF_InsertedGLASS)) "NewEnumerator6")
        (Components|StaticMesh|SetStaticMesh (Variables|/Game/Project/Core/InteractOBJ/BP_CoreOBJ.BP_CoreOBJ_C|GetStaticMesh (Variables|Default|GetREF_InsertedGLASS)) "/Game/Project/Artist/KeyObj/Mesh/SM_Slider_Single.SM_Slider_Single")
        (else
          (Components|StaticMesh|SetStaticMesh (Variables|/Game/Project/Core/InteractOBJ/BP_CoreOBJ.BP_CoreOBJ_C|GetStaticMesh (Variables|Default|GetREF_InsertedGLASS)) "/Game/Project/Artist/KeyObj/Mesh/SM_Slider_Combine.SM_Slider_Combine")
          (Default|SetInheritDiamond (Variables|Default|GetREF_InsertedGLASS)))))
    (:then_1
      (Default|UpdateTotemRTScene (Variables|/Game/Project/InteractOBJ/BP_GLASSItem.BP_GLASSItem_C|GetREF_GlassManager (Variables|Default|GetREF_InsertedGLASS)) (LocalVariables|GetL_GlassValue) (LocalVariables|GetL_SideIndex))
      (bind _previewmat (Default|ReturnRenderMatScene (Variables|/Game/Project/InteractOBJ/BP_GLASSItem.BP_GLASSItem_C|GetREF_GlassManager (Variables|Default|GetREF_InsertedGLASS)) (LocalVariables|GetL_SideIndex)))
      (Rendering|Material|SetMaterial (Variables|/Game/Project/Core/InteractOBJ/BP_CoreOBJ.BP_CoreOBJ_C|GetStaticMesh (Variables|Default|GetREF_InsertedGLASS)) 3 _previewmat)
      (Variables|/Game/Project/Core/InteractOBJ/BP_CoreITEM_GLASS.BP_CoreITEM_GLASS_C|SetGlassInsertedState (Variables|Default|GetREF_InsertedGLASS) (Variables|Default|GetGlassTAside)))
    (:then_2
      (Development|SetHiddeninGame (Variables|/Game/Project/Core/InteractOBJ/BP_CoreOBJ.BP_CoreOBJ_C|GetStaticMesh (Variables|Default|GetREF_InsertedGLASS)) false false)
      (CallFunction|PlaceOffsetOBJ (.location (Variables|/Game/Project/Core/InteractOBJ/BP_CoreITEM.BP_CoreITEM_C|GetPlaceOffset (Variables|Default|GetREF_InsertedGLASS))) (.rotation (Variables|/Game/Project/Core/InteractOBJ/BP_CoreITEM.BP_CoreITEM_C|GetPlaceOffset (Variables|Default|GetREF_InsertedGLASS))))
      (Transformation|SetActorLocation (Variables|Default|GetREF_InsertedGLASS) (Transformation|GetWorldLocation (Variables|Default|GetPlaceLocation)) false false)
      (Transformation|AttachActorToActor (Variables|Default|GetREF_InsertedGLASS) self "None" "KeepWorld" "KeepRelative" "KeepRelative" true))
    (:then_3
      (Transformation|SetActorRelativeRotation (Variables|Default|GetREF_InsertedGLASS) "0.000000,90.000000,0.000000")
      (Transformation|SetWorldScale3D (Variables|/Game/Project/Core/InteractOBJ/BP_CoreOBJ.BP_CoreOBJ_C|GetStaticMesh (Variables|Default|GetREF_InsertedGLASS)) "1.000000,1.000000,1.000000")
      (switch Utilities|FlowControl|Switch|SwitchonE_GlassSideState (Variables|Default|GetGlassTAside)
        (:NewEnumerator1
          (Utilities|Array|Add (Variables|/Game/Project/Core/InteractOBJ/BP_CoreSTAND_SET.BP_CoreSTAND_SET_C|GetChildLists (Variables|Default|GetREF_MainMachine)) (Variables|Default|GetREF_InsertedGLASS) :!label _label))
        (:NewEnumerator2
          (goto _label))
        (:NewEnumerator3
          (goto _label))
        (:NewEnumerator4
          (goto _label))
        (:NewEnumerator5
          (Utilities|Array|Add (Variables|/Game/Project/Core/InteractOBJ/BP_CoreSTAND_SET.BP_CoreSTAND_SET_C|GetChildLists (Variables|Default|GetREF_ExtractMachine)) (Variables|Default|GetREF_InsertedGLASS)))
        (:NewEnumerator6
          (Utilities|Array|Add (Variables|/Game/Project/Core/InteractOBJ/BP_CoreSTAND_SET.BP_CoreSTAND_SET_C|GetChildLists (Variables|Default|GetREF_CertifyMachine)) (Variables|Default|GetREF_InsertedGLASS)))))))

(fn UpdateGLASSCode
  (bind _ref_insertedglass (Variables|Default|GetREF_InsertedGLASS))
  (bind _updatedglass (Default|ReturnUpdatedGLASSCode (Variables|Default|GetREF_MainMachine) (Variables|Default|GetGlassTAside)))
  (Variables|/Game/Project/InteractOBJ/BP_GLASSItem.BP_GLASSItem_C|SetThisGlass (Variables|Default|GetREF_InsertedGLASS) _updatedglass)
  (bind _previewmat (Default|ReturnRenderMatScene (Variables|/Game/Project/InteractOBJ/BP_GLASSItem.BP_GLASSItem_C|GetREF_GlassManager _ref_insertedglass) 1))
  (Rendering|Material|SetMaterial (Variables|/Game/Project/Core/InteractOBJ/BP_CoreOBJ.BP_CoreOBJ_C|GetStaticMesh _ref_insertedglass) 3 _previewmat))