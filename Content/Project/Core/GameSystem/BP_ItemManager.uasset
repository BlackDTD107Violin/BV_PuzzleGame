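; BP_ItemManager renders item meshes to render-target materials through a pool of slotted scene capture rigs.
; On BeginPlay it assigns each rig in ItemRenderGroup its matching render target from RenderCameraGroupItem.
; Callers set a slot's static mesh and relative transform, then request that slot's material from MaterialGroupItem.
; Requesting a material also enables every-frame capture on that slot, which nothing here turns off.
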(event EventBeginPlay
  (CallFunction|PresetValue))

(fn ConstructionScript)

(fn PresetValue
  (for (_array_element _array_index) (Variables|Default|GetItemRenderGroup)
    (bind _output_get (Variables|/Game/Project/Core/ItemRender/BP_ItemRender.BP_ItemRender_C|SetREF_Texture%20Target _array_element (Utilities|Array|Get(acopy) (Variables|Default|GetRenderCameraGroup_Item) _array_index)))
    (Variables|/Script/Engine.SceneCaptureComponent2D|SetTextureTarget (Variables|/Game/Project/Core/ItemRender/BP_ItemRender.BP_ItemRender_C|GetSceneCaptureComponent2D _array_element) _output_get)))

(fn UpdateItemStaticMesh
  (params (TargetSlot :type Integer) (ItemToFocus :type Static%20Mesh%20Object%20Reference) (InitOffset :type Transform))
  (Variables|Default|SetSlotIndex_Item TargetSlot)
  (Components|StaticMesh|SetStaticMesh (Variables|/Game/Project/Core/ItemRender/BP_ItemRender.BP_ItemRender_C|GetStaticMesh (Utilities|Array|Get(acopy) (Variables|Default|GetItemRenderGroup) (Variables|Default|GetSlotIndex_Item))) ItemToFocus)
  (Transformation|SetRelativeTransform (Variables|/Game/Project/Core/ItemRender/BP_ItemRender.BP_ItemRender_C|GetStaticMesh (Utilities|Array|Get(acopy) (Variables|Default|GetItemRenderGroup) (Variables|Default|GetSlotIndex_Item))) InitOffset false false))

(fn ReturnRenderMatItem
  (params (TargetSlot :type Integer))
  (Variables|Default|SetSlotIndex_Item TargetSlot)
  (Variables|/Script/Engine.SceneCaptureComponent|SetbCaptureEveryFrame (Variables|/Game/Project/Core/ItemRender/BP_ItemRender.BP_ItemRender_C|GetSceneCaptureComponent2D (Utilities|Array|Get(acopy) (Variables|Default|GetItemRenderGroup) (Variables|Default|GetSlotIndex_Item))) true)
  (return (Utilities|Array|Get(acopy) (Variables|Default|GetMaterialGroup_Item) (Variables|Default|GetSlotIndex_Item))))