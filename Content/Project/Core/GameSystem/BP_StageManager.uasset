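; BP_StageManager runs a stage: it links to the main or tutorial player character, starts stage ambience and handles cutscenes and stage clear.
; On BeginPlay it applies saved BGM, SE and UI volumes through sound mix overrides.
; CallDemoFilm plays an indexed Level Sequence with movement and look locked, while Tick polls playback to clear the playing flag that blocks overlapping films.
; Clear events lock player control or show the Stage 1 clear screen and pause.
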(event Custom|Stage1ClearEvent
  (Utilities|FlowControl|Delay 0.5)
  (Default|OpenStage1Clear (Variables|/Game/ProjectDefault/FirstPerson/Blueprints/BP_FirstPersonCharacter.BP_FirstPersonCharacter_C|GetREF_CoreHUD (Variables|Default|GetPlayer)))
  (Game|SetGamePaused true))

(event Custom|CallDemoFilm
  (params (FilmCode :type Integer))
  (Variables|Default|SetFilm%20Code FilmCode)
  (if (Variables|Default|GetbPlayingFilm)
    (Development|PrintString "Film Is Playing")
    (else
      (Utilities|FlowControl|Sequence
        (:then_0
          (Default|OpenFilmHint (Variables|/Game/ProjectDefault/FirstPerson/Blueprints/BP_FirstPersonCharacter.BP_FirstPersonCharacter_C|GetREF_CoreHUD (Variables|Default|GetPlayer)) false)
          (Default|ToggleInputFilm (Variables|Default|GetPlayer) true false))
        (:then_1
          (Utilities|FlowControl|Delay 1.0)
          (bind _outactor (Sequencer|Player|CreateLevelSequencePlayer (Utilities|Array|Get(acopy) (Variables|Default|GetSequenceGroup) (Variables|Default|GetFilm%20Code)) (Utilities|Struct|MakeMovieSceneSequencePlaybackSettings false "(Value=0)" 1.0 0.0 false false true true false false false false)))
          (bind _output_get (Variables|Default|SetCurrentSequence (Variables|/Script/LevelSequence.LevelSequenceActor|GetSequencePlayer _outactor)))
          (bind _output_get_2 (Variables|/Game/ProjectDefault/FirstPerson/Blueprints/BP_FirstPersonCharacter.BP_FirstPersonCharacter_C|SetCurrentSequence (Variables|Default|GetPlayer) _output_get))
          (Sequencer|Player|Play _output_get_2 :!class /Script/MovieScene.MovieSceneSequencePlayer)
          (Variables|Default|SetbPlayingFilm true))))))

(event Custom|PlayerCtrlLockByStageClearTA
  (bind _player (Variables|Default|GetPlayer))
  (Variables|/Game/ProjectDefault/FirstPerson/Blueprints/BP_FirstPersonCharacter.BP_FirstPersonCharacter_C|SetbIgnoreESC _player true)
  (Default|TogglePlayerCtrl _player true)
  (Variables|/Script/Engine.PlayerController|SetbShowMouseCursor (Game|GetPlayerController 0) true))

(event EventBeginPlay
  (bind _returnvalue (Game|GetPlayerCharacter 0))
  (Utilities|FlowControl|Sequence
    (:then_0
      (bind _asbp_first_person_character (Utilities|Casting|CastToBP_FirstPersonCharacter _returnvalue)
        (:then
          (bind _output_get (Variables|Default|SetPlayer _asbp_first_person_character))
          (Variables|/Game/ProjectDefault/FirstPerson/Blueprints/BP_FirstPersonCharacter.BP_FirstPersonCharacter_C|SetREF_StageManager _output_get self))
        (:CastFailed
          (bind _asbp_first_person_character_tutorial (Utilities|Casting|CastToBP_FirstPersonCharacterTutorial _returnvalue))
          (Variables|Default|SetPlayerTutorial _asbp_first_person_character_tutorial))))
    (:then_1
      (Audio|SpawnSound2D (Variables|Default|GetStageAMB) 1.0 1.0 0.0 0)
      (CallFunction|PresetEachSoundValue))))

(event EventTick
  (params (DeltaSeconds :type Float%20%28single-precision%29))
  (CallFunction|FilmStateCheck))

(fn ConstructionScript)

(fn PresetEachSoundValue
  (bind _returnvalue (SaveGame|DoesSaveGameExist "BP_AudioDataSaving"))
  (if _returnvalue
    (bind _returnvalue_2 (SaveGame|LoadGamefromSlot "BP_AudioDataSaving"))
    (bind _asbp_audio_data_saving (Utilities|Casting|CastToBP_AudioDataSaving _returnvalue_2))
    (Variables|Default|SetREF_BP%20Audio%20Data%20Saving _asbp_audio_data_saving)
    (Utilities|FlowControl|Sequence
      (:then_0
        (Audio|SetSoundMixClassOverride "/Game/Project/Audio/SMix_Master.SMix_Master" "/Game/Project/Audio/SCla_BGM.SCla_BGM" (Variables|/Game/Project/Core/GameSystem/BP_AudioDataSaving.BP_AudioDataSaving_C|GetBGMvalue (Variables|Default|GetREF_BP%20Audio%20Data%20Saving)) 1.0 1.0 true)
        (Audio|PushSoundMixModifier "/Game/Project/Audio/SMix_Master.SMix_Master"))
      (:then_1
        (Audio|SetSoundMixClassOverride "/Game/Project/Audio/SMix_Master.SMix_Master" "/Game/Project/Audio/SCla_SE.SCla_SE" (Variables|/Game/Project/Core/GameSystem/BP_AudioDataSaving.BP_AudioDataSaving_C|GetSEvalue (Variables|Default|GetREF_BP%20Audio%20Data%20Saving)) 1.0 1.0 true)
        (Audio|PushSoundMixModifier "/Game/Project/Audio/SMix_Master.SMix_Master"))
      (:then_2
        (Audio|SetSoundMixClassOverride "/Game/Project/Audio/SMix_Master.SMix_Master" "/Game/Project/Audio/SCla_UISE.SCla_UISE" (Variables|/Game/Project/Core/GameSystem/BP_AudioDataSaving.BP_AudioDataSaving_C|GetUISEvalue (Variables|Default|GetREF_BP%20Audio%20Data%20Saving)) 1.0 1.0 true)
        (Audio|PushSoundMixModifier "/Game/Project/Audio/SMix_Master.SMix_Master")))
    (else
      (bind _returnvalue_3 (SaveGame|CreateSaveGameObject "/Game/Project/Core/GameSystem/BP_AudioDataSaving.BP_AudioDataSaving_C"))
      (Variables|Default|SetREF_BP%20Audio%20Data%20Saving _returnvalue_3))))

(fn FilmStateCheck
  (bind _currentsequence (Variables|Default|GetCurrentSequence))
  (if (Variables|Default|GetbPlayingFilm)
    (Utilities|IsValid _currentsequence
      (:Is%20Valid
        (Variables|Default|SetbPlayingFilm (Audio|Components|Audio|IsPlaying _currentsequence))))))