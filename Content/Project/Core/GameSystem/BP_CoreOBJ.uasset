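; BP_CoreOBJ is a core game-object actor, apparently a base class, that exposes type and identification queries.
; SetupParent caches the actor's starting transform and sets a flag when a valid parent actor exists.
; ReturnOBJType reports the stored object type, while the extract-code and object-code getters return only placeholder defaults.
; The construction script is empty, and the file has no event logic of its own.
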(fn ConstructionScript)

(fn SetupParent
  (Variables|Default|SetOriginalPos (Transformation|GetActorTransform))
  (Utilities|IsValid (Actor|GetParentActor)
    (:Is%20Valid
      (Variables|Default|SetbHasParent true))))

(fn ReturnOBJType
  (return (Variables|Default|GetThisOBJtype)))

(fn ReturnExtractCode
  (return 0))

(fn ReturnOBJCode
  (return "None"))