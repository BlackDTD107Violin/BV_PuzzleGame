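; BP_CoreTA is a core item-placement trigger area, expecting a BP_CoreSTAND_SET parent actor.
; SpawnITEM unhides the inserted BP_CoreITEM, adds that item's offset to the PlaceLocation component, then moves the item there, setting location only.
; A saved custom transform lets the placement point reset between offsets.
; PickOutITEM marks the area empty and re-enables trigger collision, while RefreshInsertedData_ITEM is an empty stub.
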(event EventBeginPlay
  (bind _asbp_core_stand_set (Utilities|Casting|CastToBP_CoreSTAND_SET (Actor|GetParentActor)))
  (Variables|Default|SetParentActor _asbp_core_stand_set))

(fn ConstructionScript)

(fn PickOutITEM
  (Variables|Default|SetbThisTAisEmpty true)
  (Collision|SetCollisionEnabled (Variables|Default|GetMain_TriggerArea) "QueryAndPhysics"))

(fn PlaceOffsetLocation
  (params (LocationOffset :type Vector) (RotatorOffset :type Rotator))
  (Transformation|SetRelativeLocationAndRotation (Variables|Default|GetPlaceLocation) LocationOffset RotatorOffset false false)
  (Variables|Default|SetCustomPlaceLocation (Transformation|GetRelativeTransform (Variables|Default|GetPlaceLocation))))

(fn PlaceOffsetOBJ
  (params (ITEMoffset :type Vector) (ITEMrotator :type Rotator))
  (Transformation|SetRelativeLocationAndRotation (Variables|Default|GetPlaceLocation) (+ ITEMoffset (Variables|/Script/Engine.SceneComponent|GetRelativeLocation (Variables|Default|GetPlaceLocation))) ITEMrotator false false))

(fn RefreshInsertedDataITEM
  (params (ITEM%20Data :type ST%20Item%20Collection%20Structure)))

(fn ResetPlaceOffset
  (Transformation|SetRelativeTransform (Variables|Default|GetPlaceLocation) (Variables|Default|GetCustomPlaceLocation) false false))

(fn SpawnITEM
  (params (InteractTarget :type Actor%20Object%20Reference))
  (bind _asbp_core_item (Utilities|Casting|CastToBP_CoreITEM InteractTarget))
  (bind _output_get (Variables|Default|SetREF_InsertedOBJ _asbp_core_item))
  (Development|SetHiddeninGame (Variables|/Game/Project/Core/InteractOBJ/BP_CoreOBJ.BP_CoreOBJ_C|GetStaticMesh _output_get) false false)
  (CallFunction|PlaceOffsetOBJ (.location (Variables|/Game/Project/Core/InteractOBJ/BP_CoreITEM.BP_CoreITEM_C|GetPlaceOffset (Variables|Default|GetREF_InsertedOBJ))) (.rotation (Variables|/Game/Project/Core/InteractOBJ/BP_CoreITEM.BP_CoreITEM_C|GetPlaceOffset (Variables|Default|GetREF_InsertedOBJ))))
  (Transformation|SetActorLocation (Variables|Default|GetREF_InsertedOBJ) (Transformation|GetWorldLocation (Variables|Default|GetPlaceLocation)) false false))