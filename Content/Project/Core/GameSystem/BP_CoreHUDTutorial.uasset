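; Tutorial HUD Blueprint that creates the core gameplay HUD and the in-game popup widgets for dialogue, hints, prompts and reading.
; BeginPlay adds all widgets to the viewport, storing the popups in GameMenusWidgetList.
; ToggleWidget keeps popups exclusive by collapsing the others, while FocusWidget and FocusGame switch visibility, input mode and cursor.
; The per-popup toggle events are empty stubs, and pause and settings widget creation is unwired.
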(event Custom|ToggleReadingP0001)

(event Custom|ToggleInteractPrompt)

(event Custom|TogglePickPrompt)

(event Custom|ToggleTrickPrompt)

(event Custom|ToggleNPCdialogue)

(event Custom|ToggleTutorialHint)

(event Custom|ToggleGamePrompt)

(event EventBeginPlay
  (bind _returnvalue (Game|Player|GetOwningPlayerController))
  (bind _returnvalue_2 (Game|Player|GetOwningPlayerController))
  (Input|SetInputModeGameOnly _returnvalue_2 false)
  ;[0.05098 0.05098 0.05098] Games - Keep showing through the Game mainly
  (bind _returnvalue_3 (UserInterface|CreateWidget "/Game/Project/Widget/WBP_Core_HUD.WBP_Core_HUD_C" _returnvalue_2))
  (bind _output_get (Variables|Default|SetREF_UI_CoreHUD _returnvalue_3))
  (UserInterface|Viewport|AddtoViewport _output_get 0)
  ;[0.05098 0.05098 0.05098] Game Menu - Popup during the game
  (bind _returnvalue_4 (UserInterface|CreateWidget "/Game/Project/Widget/WBP_NPCdialogue.WBP_NPCdialogue_C" _returnvalue))
  (bind _output_get_2 (Variables|Default|SetREF_UI_NPCdialogue _returnvalue_4))
  (Utilities|Array|Add (Variables|Default|GetGameMenus_WidgetList) _output_get_2)
  (bind _returnvalue_5 (UserInterface|CreateWidget "/Game/Project/Widget/WBP_TutorialHint.WBP_TutorialHint_C" _returnvalue))
  (bind _output_get_3 (Variables|Default|SetREF_UI_TutorialHint _returnvalue_5))
  (Utilities|Array|Add (Variables|Default|GetGameMenus_WidgetList) _output_get_3)
  (bind _returnvalue_6 (UserInterface|CreateWidget "/Game/Project/Widget/WBP_GamePrompt.WBP_GamePrompt_C" _returnvalue))
  (bind _output_get_4 (Variables|Default|SetREF_UI_GamePrompt _returnvalue_6))
  (Utilities|Array|Add (Variables|Default|GetGameMenus_WidgetList) _output_get_4)
  (bind _returnvalue_7 (UserInterface|CreateWidget "/Game/Project/Widget/WBP_InteractPrompt.WBP_InteractPrompt_C" _returnvalue))
  (bind _output_get_5 (Variables|Default|SetREF_UI_InteractPrompt _returnvalue_7))
  (Utilities|Array|Add (Variables|Default|GetGameMenus_WidgetList) _output_get_5)
  (bind _returnvalue_8 (UserInterface|CreateWidget "/Game/Project/Widget/WBP_PickPrompt.WBP_PickPrompt_C" _returnvalue))
  (bind _output_get_6 (Variables|Default|SetREF_UI_PickPrompt _returnvalue_8))
  (Utilities|Array|Add (Variables|Default|GetGameMenus_WidgetList) _output_get_6)
  (bind _returnvalue_9 (UserInterface|CreateWidget "/Game/Project/Widget/WBP_TrickPrompt.WBP_TrickPrompt_C" _returnvalue))
  (bind _output_get_7 (Variables|Default|SetREF_UI_TrickPrompt _returnvalue_9))
  (Utilities|Array|Add (Variables|Default|GetGameMenus_WidgetList) _output_get_7)
  (bind _returnvalue_10 (UserInterface|CreateWidget "/Game/Project/Widget/WBP_ReadingP0001.WBP_ReadingP0001_C" _returnvalue))
  (bind _output_get_8 (Variables|Default|SetREF_UI_ReadingP0001 _returnvalue_10))
  (Utilities|Array|Add (Variables|Default|GetGameMenus_WidgetList) _output_get_8)
  (for _array_element (Variables|Default|GetGameMenus_WidgetList)
    (UserInterface|Viewport|AddtoViewport _array_element 0)))

(fn ConstructionScript)

(fn ToggleWidget
  (params (TargetWidget :type User%20Widget%20Object%20Reference))
  (Utilities|IsValid TargetWidget
    (:Is%20Valid
      (Variables|Default|SetWidget_toFocus TargetWidget)
      (for _array_element (Variables|Default|GetGameMenus_WidgetList)
        (Utilities|IsValid _array_element
          (:Is%20Valid
            (if (== (Variables|Default|GetWidget_toFocus) _array_element)
              (if (Widget|IsVisible (Variables|Default|GetWidget_toFocus))
                (CallFunction|FocusGame)
                (else
                  (CallFunction|FocusWidget)))
              (elif (Widget|IsVisible _array_element)
                (Widget|SetVisibility _array_element "Collapsed")))))))))

(fn FocusGame
  (bind _returnvalue (Game|Player|GetOwningPlayerController))
  (Widget|SetVisibility (Variables|Default|GetWidget_toFocus) "Collapsed")
  (Input|SetInputModeGameOnly _returnvalue false)
  (Variables|/Script/Engine.PlayerController|SetbShowMouseCursor _returnvalue false))

(fn FocusWidget
  (bind _returnvalue (Game|Player|GetOwningPlayerController))
  (bind _widget_tofocus (Variables|Default|GetWidget_toFocus))
  (Widget|SetVisibility _widget_tofocus "SelfHitTestInvisible")
  (Input|SetInputModeGameandUI _returnvalue _widget_tofocus "DoNotLock" true false)
  (Variables|/Script/Engine.PlayerController|SetbShowMouseCursor _returnvalue true))