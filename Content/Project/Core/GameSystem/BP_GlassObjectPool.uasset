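; Object pool for glass actors, pre-spawning BP_GLASS_BASEtest instances at startup and recovering them when consumed.
; BeginPlay spawns a batch sized by AmountOfGlass at a fixed location, stores it in GlassPool and binds each glass's consume event.
; A consumed glass moves to the pool owner's location and attaches to that owner instead of being destroyed.
; The Blueprint contains no logic for handing glasses out.
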(event Custom|GlassReturnToPool
  (params (Glass :type BP%20GLASS%20BAS%20Etest%20Object%20Reference))
  (bind _returnvalue (Components|GetOwner))
  (Transformation|SetActorLocation Glass (Transformation|GetActorLocation _returnvalue) false false)
  (Transformation|AttachActorToActor Glass _returnvalue "None" "KeepWorld" "KeepWorld" "KeepWorld" true))

(event EventBeginPlay
  (for _index (range 0 (Variables|Default|GetAmountOfGlass))
    (bind _returnvalue (Game|SpawnActorfromClass "/Game/Project/InteractOBJ/BP_GLASS_BASEtest.BP_GLASS_BASEtest_C" (Math|Transform|MakeTransform "500.000000,0.000000,0.000000" "0, 0, 0" "1.000000,1.000000,1.000000") "Undefined" 0 "NewEnumerator6" false false 0))
    (EventDispatchers|BindEventtoConsumeThisGlass _returnvalue (delegate Custom|GlassReturnToPool))
    (Utilities|Array|Add (Variables|Default|GetGlassPool) _returnvalue)))

(fn ConstructionScript)