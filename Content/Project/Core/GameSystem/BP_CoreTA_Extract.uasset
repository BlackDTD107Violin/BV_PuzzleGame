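; BP_CoreTA_Extract is a placement trigger area that receives items for extraction and links them to the REFS9008 object.
; On insertion it spawns the item, sends its data to REFS9008 as an extract code and caches float settings from the item's extract component.
; Film_ExtractFloating runs a timeline that lifts and rotates the item, with an event track playing its drop sound.
; Picking the item out clears REFS9008's set flag.
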(event Custom|Film_ExtractFloating
  (bind _placelocation (Variables|Default|GetPlaceLocation))
  (bind _returnvalue (Transformation|GetWorldLocation _placelocation))
  (Variables|Default|SetBaseAngle (Transformation|GetActorRotation (Variables|Default|GetREF_InsertedOBJ)))
  (Utilities|IsValid (Variables|Default|GetREF_InsertedOBJ)
    (:Is%20Valid
      (bind (_direction _floatheight _floatangle) (Timeline|OBJFloating PlayFromStart)
        (:Update
          (Transformation|SetActorLocation (Variables|Default|GetREF_InsertedOBJ) (Math|Vector|MakeVector (.x _returnvalue) (.y _returnvalue) (Math|Float|Lerp (.z _returnvalue) (+ (.z _returnvalue) (Variables|Default|GetFloatHeight)) _floatheight)) false false)
          (Transformation|SetActorRotation (Variables|Default|GetREF_InsertedOBJ) (Math|Rotator|Lerp(Rotator) (Variables|Default|GetBaseAngle) (Variables|Default|GetFloat%20Angle) _floatangle)))
        (:SEPlay
          (bind _asbp_core_item_extract (Utilities|Casting|CastToBP_CoreITEM_EXTRACT (Variables|Default|GetREF_InsertedOBJ)))
          (Audio|SpawnSoundAttached (Variables|/Game/Project/Core/InteractOBJ/AC_ExtractComponent.AC_ExtractComponent_C|GetExtractDropSE (Variables|/Game/Project/Core/InteractOBJ/BP_CoreITEM_EXTRACT.BP_CoreITEM_EXTRACT_C|GetAC_ExtractComponent _asbp_core_item_extract)) (Variables|Default|GetPlaceLocation) "None" "0, 0, 0" "0, 0, 0" "KeepRelativeOffset" false 1.0 1.0 0.0 0 0))))))

(event EventBeginPlay
  (|CallParentFunction) ; This node is disabled and will not be called.\nDrag off pins to build functionality.
)

(event Collision|EventActorBeginOverlap
  (params (OtherActor :type Actor%20Object%20Reference))
  (|CallParentFunction OtherActor) ; This node is disabled and will not be called.\nDrag off pins to build functionality.
)

(event EventTick
  (params (DeltaSeconds :type Float%20%28single-precision%29))
  (|CallParentFunction DeltaSeconds) ; This node is disabled and will not be called.\nDrag off pins to build functionality.
)

(fn ConstructionScript
  (|CallParentFunction))

(fn PickOutITEM
  (|CallParentFunction)
  (Variables|/Game/Project/InteractOBJ/BP_S9008.BP_S9008_C|SetbOBJIsSet (Variables|Default|GetREF_S9008) false))

(fn RefreshInsertedDataITEM
  (params (ITEM%20Data :type ST%20Item%20Collection%20Structure))
  (Variables|Default|SetInsertedITEMData ITEM%20Data)
  (Utilities|FlowControl|Sequence
    (:then_0
      (CallFunction|SpawnITEM (.TargetItemActor (Utilities|Struct|BreakST_ItemCollection (Variables|Default|GetInsertedITEMData))))
      (Rendering|SetActorHiddenInGame (.TargetItemActor (Utilities|Struct|BreakST_ItemCollection (Variables|Default|GetInsertedITEMData))) false)
      (Collision|SetActorEnableCollision (.TargetItemActor (Utilities|Struct|BreakST_ItemCollection (Variables|Default|GetInsertedITEMData))) true)
      (Audio|SpawnSoundAttached (.PlaceSE (Utilities|Struct|BreakST_ItemCollection (Variables|Default|GetInsertedITEMData))) (Variables|Default|GetMain_TriggerArea) "None" "0, 0, 0" "0, 0, 0" "KeepRelativeOffset" false 1.0 1.0 0.0 0 0))
    (:then_1
      (Default|ReceiveOBJExtractCode (Variables|Default|GetREF_S9008) (Variables|Default|GetInsertedITEMData))
      (Variables|Default|SetbThisTAisEmpty false)
      (bind _asbp_core_item_extract (Utilities|Casting|CastToBP_CoreITEM_EXTRACT (Utilities|Struct|BreakST_ItemCollection (Variables|Default|GetInsertedITEMData))))
      (Variables|/Game/Project/Core/InteractOBJ/BP_CoreITEM_EXTRACT.BP_CoreITEM_EXTRACT_C|SetCurrentInsertedExtractTA _asbp_core_item_extract self))))

(fn SpawnITEM
  (params (InteractTarget :type Actor%20Object%20Reference))
  (|CallParentFunction InteractTarget)
  (Utilities|FlowControl|Sequence
    (:then_0
      (bind _asbp_core_item_extract (Utilities|Casting|CastToBP_CoreITEM_EXTRACT (Variables|Default|GetREF_InsertedOBJ)))
      (Variables|Default|SetFloatHeight (Variables|/Game/Project/Core/InteractOBJ/AC_ExtractComponent.AC_ExtractComponent_C|GetExtractFloatHeight (Variables|/Game/Project/Core/InteractOBJ/BP_CoreITEM_EXTRACT.BP_CoreITEM_EXTRACT_C|GetAC_ExtractComponent _asbp_core_item_extract)))
      (Variables|Default|SetFloat%20Angle (Variables|/Game/Project/Core/InteractOBJ/AC_ExtractComponent.AC_ExtractComponent_C|GetExtractFloatAngle (Variables|/Game/Project/Core/InteractOBJ/BP_CoreITEM_EXTRACT.BP_CoreITEM_EXTRACT_C|GetAC_ExtractComponent _asbp_core_item_extract))))
    (:then_1
      (Utilities|Array|Add (Variables|/Game/Project/Core/InteractOBJ/BP_CoreSTAND_SET.BP_CoreSTAND_SET_C|GetChildLists (Variables|Default|GetREF_S9008)) (Variables|Default|GetREF_InsertedOBJ)))))