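; Main menu manager actor that sets up the menu screen when play begins.
; BeginPlay creates and stores WBP_MainMenu, adds it to the viewport, and shows the mouse cursor for the first player controller.
; It also turns off its own camera-component lookup and switches the view target to StaticCameraMenu.
; A UI-only input mode call focused on the menu is present but unconnected, so it never runs.
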(event EventBeginPlay
  (Utilities|FlowControl|Sequence
    (:then_0
      (bind _returnvalue (UserInterface|CreateWidget "/Game/Project/Widget/WBP_MainMenu.WBP_MainMenu_C"))
      (bind _output_get (Variables|Default|SetMainMenuREF _returnvalue))
      (UserInterface|Viewport|AddtoViewport _returnvalue 0))
    (:then_1
      (Variables|Default|SetbFindCameraComponentWhenViewTarget false)
      (Game|Player|SetViewTargetwithBlend (Game|GetPlayerController 0) (Variables|Default|GetStaticCamera_Menu) 0.0 "VTBlend_Cubic" 0.0 false))
    (:then_2
      (Variables|/Script/Engine.PlayerController|SetbShowMouseCursor (Game|GetPlayerController 0) true))))

(fn ConstructionScript)