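; BP_R0001 is a child Blueprint for the READ item with serial code "R0001", tied to the tutorial first-person character.
; Attaching it to the hand notifies the player through InteractwithREAD with that code.
; Repos restores its original transform and, if it has a parent, snaps it to the serial-named socket on the stored root, then notifies the player again.
; The first such reattachment also advances the tutorial and clears the game prompt.
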(event EventBeginPlay
  (|CallParentFunction)
  (Variables|Default|SetREADSerialCode "R0001")
  (bind _asbp_first_person_character_tutorial (Utilities|Casting|CastToBP_FirstPersonCharacterTutorial (Game|GetPlayerCharacter 0)))
  (Variables|Default|SetPlayer _asbp_first_person_character_tutorial))

(event EventAttachtoHand
  (params (InteractTarget :type Actor%20Component%20Object%20Reference))
  (Default|InteractwithREAD (Variables|Default|GetPlayer) (Variables|Default|GetREADSerialCode)))

(event EventSetTempPos
  (params (Root :type Static%20Mesh%20Component%20Object%20Reference))
  ;[0.05098 0.05098 0.05098] Temp Repos will execute when the root parent is moving
  (Variables|Default|SetReAttach Root)
  (Development|PrintString "Success"))

(event EventRepos
  (bind _player (Variables|Default|GetPlayer))
  (Transformation|SetActorRelativeTransform (Variables|Default|GetOriginalPos) false false)
  (if (Variables|Default|GetbHasParent)
    (Transformation|AttachComponentToComponent (Variables|Default|GetReAttach) (Variables|Default|GetREADSerialCode) "SnapToTarget" "KeepWorld" "KeepWorld" true)
    (Default|InteractwithREAD (Variables|Default|GetPlayer) (Variables|Default|GetREADSerialCode))
    (if (not (Variables|Default|GetbHasTriggerTutor))
      (Variables|Default|SetbHasTriggerTutor true)
      (Default|ArriveTutorialTA _player)
      (Default|ClearGamePromptUIView _player))))

(fn ConstructionScript
  (|CallParentFunction))