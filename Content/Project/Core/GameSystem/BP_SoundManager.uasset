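; Sound manager Blueprint that starts the stage ambience and restores saved audio volume settings at BeginPlay.
; It loads the BP_AudioDataSaving slot and pushes SMix_Master class overrides for the BGM, SE and UI SE sound classes using the saved values.
; When no save exists, it only creates a new save object and keeps a reference, without applying or writing volumes.
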(event EventBeginPlay
  (Audio|SpawnSound2D (Variables|Default|GetStageAMB) 1.0 1.0 0.0 0)
  (CallFunction|PresetEachSoundValue))

(fn ConstructionScript)

(fn PresetEachSoundValue
  (bind _returnvalue (SaveGame|DoesSaveGameExist "BP_AudioDataSaving"))
  (if _returnvalue
    (bind _returnvalue_2 (SaveGame|LoadGamefromSlot "BP_AudioDataSaving"))
    (bind _asbp_audio_data_saving (Utilities|Casting|CastToBP_AudioDataSaving _returnvalue_2))
    (Variables|Default|SetREF_BP%20Audio%20Data%20Saving _asbp_audio_data_saving)
    (Utilities|FlowControl|Sequence
      (:then_0
        (Audio|SetSoundMixClassOverride "/Game/Project/Audio/SMix_Master.SMix_Master" "/Game/Project/Audio/SCla_BGM.SCla_BGM" (Variables|/Game/Project/Core/GameSystem/BP_AudioDataSaving.BP_AudioDataSaving_C|GetBGMvalue (Variables|Default|GetREF_BP%20Audio%20Data%20Saving)) 1.0 1.0 true)
        (Audio|PushSoundMixModifier "/Game/Project/Audio/SMix_Master.SMix_Master"))
      (:then_1
        (Audio|SetSoundMixClassOverride "/Game/Project/Audio/SMix_Master.SMix_Master" "/Game/Project/Audio/SCla_SE.SCla_SE" (Variables|/Game/Project/Core/GameSystem/BP_AudioDataSaving.BP_AudioDataSaving_C|GetSEvalue (Variables|Default|GetREF_BP%20Audio%20Data%20Saving)) 1.0 1.0 true)
        (Audio|PushSoundMixModifier "/Game/Project/Audio/SMix_Master.SMix_Master"))
      (:then_2
        (Audio|SetSoundMixClassOverride "/Game/Project/Audio/SMix_Master.SMix_Master" "/Game/Project/Audio/SCla_UISE.SCla_UISE" (Variables|/Game/Project/Core/GameSystem/BP_AudioDataSaving.BP_AudioDataSaving_C|GetUISEvalue (Variables|Default|GetREF_BP%20Audio%20Data%20Saving)) 1.0 1.0 true)
        (Audio|PushSoundMixModifier "/Game/Project/Audio/SMix_Master.SMix_Master")))
    (else
      (bind _returnvalue_3 (SaveGame|CreateSaveGameObject "/Game/Project/Core/GameSystem/BP_AudioDataSaving.BP_AudioDataSaving_C"))
      (Variables|Default|SetREF_BP%20Audio%20Data%20Saving _returnvalue_3))))