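; BP_CoreOBJ_PICKUP is a core-object Blueprint for pickups, setting its object type enum on BeginPlay.
; SetupParent caches the actor's original transform and flags whether it has a valid parent actor.
; ReturnOBJCode returns placeholder serial and extract key codes, and the construction script only calls its parent's.
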(event EventBeginPlay
  (Variables|Default|SetThisOBJtype "NewEnumerator2"))

(fn ConstructionScript
  (|CallParentFunction))

(fn SetupParent
  (Variables|Default|SetOriginalPos (Transformation|GetActorTransform))
  (Utilities|IsValid (Actor|GetParentActor)
    (:Is%20Valid
      (Variables|Default|SetbHasParent true))))

(fn ReturnOBJCode
  (return "None" 0))