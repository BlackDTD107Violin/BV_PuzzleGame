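; Manager actor that pools glass items and manages the render-to-texture setups that draw their totems.
; On BeginPlay it pre-spawns the glass pool, handed out by a wrapping index; consumed glasses detach and move back to the manager.
; Base, Unite and Scene groups pair scene-capture renderers with render targets, with functions to update totems, enable capture, return materials and toggle spline states.
; Two test layout functions are never run.
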(event Custom|GlassReturnToPool
  (params (Glass :type BP%20GLASS%20Item%20Object%20Reference))
  (Transformation|SetActorLocation Glass (Transformation|GetActorLocation) false false)
  (Transformation|DetachFromActor Glass "KeepRelative" "KeepRelative" "KeepRelative"))

(event EventBeginPlay
  (for _index (range 0 (Variables|Default|GetAmountOfGlass))
    (bind _returnvalue (Game|SpawnActorfromClass "/Game/Project/InteractOBJ/BP_GLASSItem.BP_GLASSItem_C" (Math|Transform|MakeTransform (+ (Transformation|GetActorLocation) "10000.000000,0.000000,0.000000") "0, 0, 0" "1.000000,1.000000,1.000000") "Undefined" 0 "NewEnumerator6" 0))
    (EventDispatchers|BindEventtoConsumeThisGlass _returnvalue (delegate Custom|GlassReturnToPool))
    (Variables|/Game/Project/InteractOBJ/BP_GLASSItem.BP_GLASSItem_C|SetREF_GlassManager _returnvalue self)
    (bind _returnvalue_2 (Utilities|Array|Add (Variables|Default|GetGlassPool) _returnvalue)))
  (CallFunction|PresetValue))

(fn ConstructionScript)

(fn 0420Test
  (params (Index :type Integer))
  (bind _glasspool (Variables|Default|GetGlassPool))
  (bind _output (Utilities|Array|Get(acopy) _glasspool Index))
  (if (< Index 12)
    (Variables|/Game/Project/InteractOBJ/BP_GLASSItem.BP_GLASSItem_C|SetThisGlass _output (Utilities|Struct|MakeST_GlassData _output -1 0 0 0 0))
    (Transformation|SetActorLocation _output (Math|Vector|MakeVector 292.056303 (+ (LocalVariables|GetNewLocalVar) (* Index 40)) 89.045886) false false)
    (Transformation|SetActorRotation _output "90.000000,180.000000,180.000000")
    (Utilities|Array|Add (.glassvalue (Variables|/Game/Project/InteractOBJ/BP_GLASSItem.BP_GLASSItem_C|GetThisGlass _output)) (Utilities|Struct|MakeST_GlassValue "/Game/Developers/LinYanChen/Image/IMS_Testpng3.IMS_Testpng3" "/Game/Project/Effects/BP_Sp1001_Fire.BP_Sp1001_Fire_C" 0 1 0 3))
    (else
      (Variables|Default|SetGlassIndex 12))))

(fn 0601TestPasswordTotemSpawn
  (params (Index :type Integer))
  (bind _output_get (LocalVariables|SetL_Index Index))
  (if (< _output_get 4)
    (bind _output_get_2 (LocalVariables|SetL_TargetGlass (Utilities|Array|Get(acopy) (Variables|Default|GetGlassPool) (LocalVariables|GetL_Index))))
    (Variables|/Game/Project/InteractOBJ/BP_GLASSItem.BP_GLASSItem_C|SetThisGlass _output_get_2 (Utilities|Struct|MakeST_GlassData _output_get_2 -1 0 0 0 0))
    (Transformation|SetActorLocation (LocalVariables|GetL_TargetGlass) (Math|Vector|MakeVector 292.056303 (+ (LocalVariables|GetNewLocalVar) (* (LocalVariables|GetL_Index) 40)) 89.045886) false false)
    (Transformation|SetActorRotation (LocalVariables|GetL_TargetGlass) "90.000000,180.000000,180.000000")
    (Utilities|Array|Add (.glassvalue (Variables|/Game/Project/InteractOBJ/BP_GLASSItem.BP_GLASSItem_C|GetThisGlass (LocalVariables|GetL_TargetGlass))) (Utilities|Select :Index (LocalVariables|GetL_Index) :Option%200 (Utilities|Struct|MakeST_GlassValue "/Game/Developers/LinYanChen/Image/IMS_Testpng3.IMS_Testpng3" "/Game/Project/Effects/BP_Sp1001_Fire.BP_Sp1001_Fire_C" 0 1 0 6) :Option%201 (Utilities|Struct|MakeST_GlassValue "/Game/Developers/LinYanChen/Image/IMS_Testpng3.IMS_Testpng3" "/Game/Project/Effects/BP_Sp1002_Catalyst.BP_Sp1002_Catalyst_C" 0 1 0 5) :Option%202 (Utilities|Struct|MakeST_GlassValue "/Game/Developers/LinYanChen/Image/IMS_Testpng3.IMS_Testpng3" "/Game/Project/Effects/BP_Sp1003_Fuel.BP_Sp1003_Fuel_C" 0 2 0 5) :Option%203 (Utilities|Struct|MakeST_GlassValue "/Game/Developers/LinYanChen/Image/IMS_Testpng3.IMS_Testpng3" "/Game/Project/Effects/BP_Sp1004_Sun.BP_Sp1004_Sun_C" 0 6 3)))
    (else
      (Variables|Default|SetGlassIndex 4))))

(fn PresetValue
  (Utilities|FlowControl|Sequence
    (:then_0
      (for (_array_element _array_index) (Variables|Default|GetGlassRenderGroup_Base)
        (bind _output_get (Variables|/Game/Project/Core/GlassRender_Base/BP_GlassRender_Base.BP_GlassRender_Base_C|SetREF_Texture%20Target _array_element (Utilities|Array|Get(acopy) (Variables|Default|GetRenderCameraGroup_Base) _array_index)))
        (Variables|/Script/Engine.SceneCaptureComponent2D|SetTextureTarget (Variables|/Game/Project/Core/GlassRender_Base/BP_GlassRender_Base.BP_GlassRender_Base_C|GetSceneCaptureComponent2D _array_element) _output_get)))
    (:then_1
      (for (_array_element_2 _array_index_2) (Variables|Default|GetGlassRenderGroup_Unite)
        (bind _output_get_2 (Variables|/Game/Project/Core/GlassRender_Unite/BP_GlassRender_Unite.BP_GlassRender_Unite_C|SetREF_Texture%20Target _array_element_2 (Utilities|Array|Get(acopy) (Variables|Default|GetRenderCameraGroup_Unite) _array_index_2)))
        (Variables|/Script/Engine.SceneCaptureComponent2D|SetTextureTarget (Variables|/Game/Project/Core/GlassRender_Unite/BP_GlassRender_Unite.BP_GlassRender_Unite_C|GetSceneCaptureComponent2D _array_element_2) _output_get_2)))
    (:then_2
      (for (_array_element_3 _array_index_3) (Variables|Default|GetGlassRenderGroup_Scene)
        (bind _output_get_3 (Variables|/Game/Project/Core/GlassRender_Unite/BP_GlassRender_Unite.BP_GlassRender_Unite_C|SetREF_Texture%20Target _array_element_3 (Utilities|Array|Get(acopy) (Variables|Default|GetRenderCameraGroup_Scene) _array_index_3)))
        (Variables|/Script/Engine.SceneCaptureComponent2D|SetTextureTarget (Variables|/Game/Project/Core/GlassRender_Unite/BP_GlassRender_Unite.BP_GlassRender_Unite_C|GetSceneCaptureComponent2D _array_element_3) _output_get_3)))))

(fn AcquireGlassfromPool
  (bind _glasspool (Variables|Default|GetGlassPool))
  (if (> (Utilities|Array|Length _glasspool) 0)
    (Utilities|IsValid (Utilities|Array|Get(acopy) _glasspool (Variables|Default|GetGlassIndex))
      (:Is%20Valid
        (bind _result (Math|Integer|IncrementInt (Variables|Default|GetGlassIndex))
          (:%20%20
            (bind _output_get (Variables|Default|SetGlassIndex _result))
            (if (== _output_get (Variables|Default|GetAmountOfGlass))
              (Variables|Default|SetGlassIndex 0))
            (return (Utilities|Array|Get(acopy) _glasspool (Variables|Default|GetGlassIndex))))))
      (:Is%20Not%20Valid
        _)))
  (return 0))

(fn UpdateTotemRTBase
  (params (ExtractData :type ST%20Glass%20Value%20Structure) (TargetSlot :type Integer))
  (Variables|Default|SetSlotIndex_Base TargetSlot)
  (Default|UpdateRenderer (Utilities|Array|Get(acopy) (Variables|Default|GetGlassRenderGroup_Base) (Variables|Default|GetSlotIndex_Base)) ExtractData))

(fn ReturnRenderMatBase
  (params (TargetSlot :type Integer))
  (Variables|Default|SetSlotIndex_Base TargetSlot)
  (Variables|/Script/Engine.SceneCaptureComponent|SetbCaptureEveryFrame (Variables|/Game/Project/Core/GlassRender_Base/BP_GlassRender_Base.BP_GlassRender_Base_C|GetSceneCaptureComponent2D (Utilities|Array|Get(acopy) (Variables|Default|GetGlassRenderGroup_Base) (Variables|Default|GetSlotIndex_Base))) true)
  (return (Utilities|Array|Get(acopy) (Variables|Default|GetMaterialGroup_Base) (Variables|Default|GetSlotIndex_Base))))

(fn UpdateTotemRTUnite
  (params (ValueGroups :type Array%20of%20ST%20Glass%20Value%20Structures) (TargetSlot :type Integer))
  (Variables|Default|SetSlotIndex_Unite TargetSlot)
  (Default|UpdateRenderer (Utilities|Array|Get(acopy) (Variables|Default|GetGlassRenderGroup_Unite) (Variables|Default|GetSlotIndex_Unite)) ValueGroups))

(fn ReturnRenderMatUnite
  (params (TargetSlot :type Integer))
  (Variables|Default|SetSlotIndex_Unite TargetSlot)
  (Variables|/Script/Engine.SceneCaptureComponent|SetbCaptureEveryFrame (Variables|/Game/Project/Core/GlassRender_Unite/BP_GlassRender_Unite.BP_GlassRender_Unite_C|GetSceneCaptureComponent2D (Utilities|Array|Get(acopy) (Variables|Default|GetGlassRenderGroup_Unite) (Variables|Default|GetSlotIndex_Unite))) true)
  (return (Utilities|Array|Get(acopy) (Variables|Default|GetMaterialGroup_Unite) (Variables|Default|GetSlotIndex_Unite))))

(fn UpdateTotemRTScene
  (params (ValueGroups :type Array%20of%20ST%20Glass%20Value%20Structures) (SideState :type Integer))
  (LocalVariables|SetL_SideIndex SideState)
  (Default|UpdateRenderer (Utilities|Array|Get(acopy) (Variables|Default|GetGlassRenderGroup_Scene) (LocalVariables|GetL_SideIndex)) ValueGroups))

(fn ReturnRenderMatScene
  (params (SideState :type Integer))
  (LocalVariables|SetL_SideIndex SideState)
  (Variables|/Script/Engine.SceneCaptureComponent|SetbCaptureEveryFrame (Variables|/Game/Project/Core/GlassRender_Unite/BP_GlassRender_Unite.BP_GlassRender_Unite_C|GetSceneCaptureComponent2D (Utilities|Array|Get(acopy) (Variables|Default|GetGlassRenderGroup_Scene) (LocalVariables|GetL_SideIndex))) true)
  (return (Utilities|Array|Get(acopy) (Variables|Default|GetMaterialGroup_Scene) (LocalVariables|GetL_SideIndex))))

(fn SwitchStateRenderMatBase
  (params (bIsEnable :type Boolean))
  (for _array_element (Variables|Default|GetGlassRenderGroup_Base)
    (Default|SwitchEachSplineState _array_element bIsEnable)))

(fn SwitchStateRenderMatUnite
  (params (bIsEnable :type Boolean))
  (for _array_element (Variables|Default|GetGlassRenderGroup_Unite)
    (Default|SwitchEachSplineState _array_element bIsEnable)))

(fn SwitchStateRenderMatScene
  (params (Target :type Integer) (bIsEnable :type Boolean))
  (if (>= Target 0)
    (Default|SwitchEachSplineState (Utilities|Array|Get(acopy) (Variables|Default|GetGlassRenderGroup_Scene) Target) bIsEnable)))