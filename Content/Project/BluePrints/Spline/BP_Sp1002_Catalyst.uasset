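; Catalyst spline effect actor that moves five small runner components along five splines, with a Niagara color that can be switched by glass side.
; On BeginPlay a timeline drives a normalized alpha that places each runner at that fraction of its spline's length, matching location and rotation.
; The construction script gathers splines, runners and Niagara components into arrays.
; SwitchTotemEffectByInputSide sets TotemColor on all Niagara systems, red for either mixer side and yellow for Calculate.
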(event EventBeginPlay
  (bind _spline3 (Variables|Default|GetSpline3))
  (bind _spline2 (Variables|Default|GetSpline2))
  (bind _spline4 (Variables|Default|GetSpline4))
  (bind _spline (Variables|Default|GetSpline))
  (bind _spline1 (Variables|Default|GetSpline1))
  (|CallParentFunction)
  (bind _animtest (Timeline|Timeline PlayFromStart)
    (:Update
      (Variables|Default|SetAnim%20Test _animtest)
      (Utilities|FlowControl|Sequence
        (:then_0
          (Transformation|SetRelativeTransform (Variables|Default|GetRunner) (Math|Transform|MakeTransform (Spline|GetLocationatDistanceAlongSpline _spline (* (Variables|Default|GetAnim%20Test) (Spline|GetSplineLength _spline)) "Local") (Spline|GetRotationatDistanceAlongSpline _spline (* (Variables|Default|GetAnim%20Test) (Spline|GetSplineLength _spline)) "Local") "0.025000,0.025000,0.025000") false false))
        (:then_1
          (Transformation|SetRelativeTransform (Variables|Default|GetRunner1) (Math|Transform|MakeTransform (Spline|GetLocationatDistanceAlongSpline _spline1 (* (Variables|Default|GetAnim%20Test) (Spline|GetSplineLength _spline1)) "Local") (Spline|GetRotationatDistanceAlongSpline _spline1 (* (Variables|Default|GetAnim%20Test) (Spline|GetSplineLength _spline1)) "Local") "0.025000,0.025000,0.025000") false false))
        (:then_2
          (Transformation|SetRelativeTransform (Variables|Default|GetRunner2) (Math|Transform|MakeTransform (Spline|GetLocationatDistanceAlongSpline _spline2 (* (Variables|Default|GetAnim%20Test) (Spline|GetSplineLength _spline2)) "Local") (Spline|GetRotationatDistanceAlongSpline _spline2 (* (Variables|Default|GetAnim%20Test) (Spline|GetSplineLength _spline2)) "Local") "0.025000,0.025000,0.025000") false false))
        (:then_3
          (Transformation|SetRelativeTransform (Variables|Default|GetRunner4) (Math|Transform|MakeTransform (Spline|GetLocationatDistanceAlongSpline _spline4 (* (Variables|Default|GetAnim%20Test) (Spline|GetSplineLength _spline4)) "Local") (Spline|GetRotationatDistanceAlongSpline _spline4 (* (Variables|Default|GetAnim%20Test) (Spline|GetSplineLength _spline4)) "Local") "0.025000,0.025000,0.025000") false false))
        (:then_4
          (Transformation|SetRelativeTransform (Variables|Default|GetRunner3) (Math|Transform|MakeTransform (Spline|GetLocationatDistanceAlongSpline _spline3 (* (Variables|Default|GetAnim%20Test) (Spline|GetSplineLength _spline3)) "Local") (Spline|GetRotationatDistanceAlongSpline _spline3 (* (Variables|Default|GetAnim%20Test) (Spline|GetSplineLength _spline3)) "Local") "0.025000,0.025000,0.025000") false false))))))

(fn ConstructionScript
  (|CallParentFunction)
  (Utilities|FlowControl|Sequence
    (:then_0
      (Utilities|Array|Add (Variables|Default|GetSplineGroups) (Variables|Default|GetSpline))
      (Utilities|Array|Add (Variables|Default|GetSplineGroups) (Variables|Default|GetSpline1))
      (Utilities|Array|Add (Variables|Default|GetSplineGroups) (Variables|Default|GetSpline2))
      (Utilities|Array|Add (Variables|Default|GetSplineGroups) (Variables|Default|GetSpline3))
      (Utilities|Array|Add (Variables|Default|GetSplineGroups) (Variables|Default|GetSpline4)))
    (:then_1
      (Utilities|Array|Add (Variables|Default|GetRunnerGroups) (Variables|Default|GetRunner))
      (Utilities|Array|Add (Variables|Default|GetRunnerGroups) (Variables|Default|GetRunner1))
      (Utilities|Array|Add (Variables|Default|GetRunnerGroups) (Variables|Default|GetRunner2))
      (Utilities|Array|Add (Variables|Default|GetRunnerGroups) (Variables|Default|GetRunner3))
      (Utilities|Array|Add (Variables|Default|GetRunnerGroups) (Variables|Default|GetRunner4)))
    (:then_2
      (Utilities|Array|Add (Variables|Default|GetNiagaraGroups) (Variables|Default|GetNiagara))
      (Utilities|Array|Add (Variables|Default|GetNiagaraGroups) (Variables|Default|GetNiagara1))
      (Utilities|Array|Add (Variables|Default|GetNiagaraGroups) (Variables|Default|GetNiagara2))
      (Utilities|Array|Add (Variables|Default|GetNiagaraGroups) (Variables|Default|GetNiagara3))
      (Utilities|Array|Add (Variables|Default|GetNiagaraGroups) (Variables|Default|GetNiagara4)))))

(fn SwitchTotemEffectbyInputSide
  (params (GlassSide :type E_GlassSideState%20Enum :default "NewEnumerator0"))
  (switch Utilities|FlowControl|Switch|SwitchonE_GlassSideState GlassSide
    (:NewEnumerator1
      (for _array_element (Variables|Default|GetNiagaraGroups) :!label _label
        (Niagara|SetNiagaraVariable(Vector3) _array_element "TotemColor" "1.000000,0.000000,0.000000")))
    (:NewEnumerator2
      (goto _label))
    (:NewEnumerator4
      (for _array_element_2 (Variables|Default|GetNiagaraGroups)
        (Niagara|SetNiagaraVariable(Vector3) _array_element_2 "TotemColor" "1.000000,0.912126,0.000000")))))