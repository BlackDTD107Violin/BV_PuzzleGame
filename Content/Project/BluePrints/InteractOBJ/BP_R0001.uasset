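; BP_R0001 is an inspectable paper object in the world, built on a parent class.
; It caches the first-person tutorial character on BeginPlay.
; Entering inspection hides the mesh and exiting shows it again, each playing an attached paper pick/place sound.
; On entering, it also calls the player's InteractwithREAD while HasTriggerTutor is false, a flag this graph never sets.
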(event EventBeginPlay
  (|CallParentFunction)
  (bind _asbp_first_person_character_tutorial (Utilities|Casting|CastToBP_FirstPersonCharacterTutorial (Game|GetPlayerCharacter 0)))
  (Variables|Default|SetPlayer _asbp_first_person_character_tutorial))

(event EventEnterInspector
  (Audio|SpawnSoundAttached "/Game/Project/Audio/MetaSoundSource/SE/MSS_Pick_Place_Paper_1.MSS_Pick_Place_Paper_1" (Variables|Default|GetStaticMesh) "None" "0, 0, 0" "0, 0, 0" "KeepRelativeOffset" false 1.0 1.0 0.0 0 0)
  (Development|SetHiddeninGame (Variables|Default|GetStaticMesh) true false)
  (if (not (Variables|Default|GetbHasTriggerTutor))
    (Default|InteractwithREAD (Variables|Default|GetPlayer))))

(event EventExitInspector
  (Development|SetHiddeninGame (Variables|Default|GetStaticMesh) false false)
  (Audio|SpawnSoundAttached "/Game/Project/Audio/MetaSoundSource/SE/MSS_Pick_Place_Paper_1.MSS_Pick_Place_Paper_1" (Variables|Default|GetStaticMesh) "None" "0, 0, 0" "0, 0, 0" "KeepRelativeOffset" false 1.0 1.0 0.0 0 0))

(fn ConstructionScript
  (|CallParentFunction))