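; Zoomable interactable paper scroll (S1001) that the player drags open to reveal glass totem previewers.
; Tick moves the handle by vertical mouse direction and maps its position to the geometry-cache start time offset to animate unrolling.
; On release it eases open if nearly there, otherwise closed, with scroll audio following motion; full opening locks it.
; Construction collects child-actor previewers, which receive glass values through AssignTotemPreviewer, with one side also updating a render-target scene.
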(event OnClicked(ScrollHandle)
  (params (TouchedComponent :type Primitive%20Component%20Object%20Reference) (ButtonPressed :type Key%20Structure))
  ;[1 1 1] Mesh Control Event
  (if (Variables|Default|GetbScrollIsFinish)
    (Variables|Default|SetbIsDragScroll false)
    (else
      (Variables|Default|SetbIsDragScroll true)
      (Variables|/Game/ProjectDefault/FirstPerson/Blueprints/BP_FirstPersonCharacter.BP_FirstPersonCharacter_C|SetCurrentInteract (Variables|Default|GetPlayer) self))))

(event EventBeginPlay
  (|CallParentFunction))

(event EventZoomin
  (params (ZoomComponent :type Actor%20Component%20Object%20Reference))
  (|CallParentFunction ZoomComponent)
  (CallFunction|SwitchMeshCollisionProfile true))

(event EventZoomOut
  (|CallParentFunction))

(event EventInteractEnd
  (Variables|/Game/ProjectDefault/FirstPerson/Blueprints/BP_FirstPersonCharacter.BP_FirstPersonCharacter_C|SetCurrentInteract (Variables|Default|GetPlayer) self)
  (Variables|Default|SetbSoundPlaying false)
  (Variables|Default|SetbIsDragScroll false))

(event EventTick
  (params (DeltaSeconds :type Float%20%28single-precision%29))
  (if (not (Variables|Default|GetbScrollIsFinish))
    (if (Variables|Default|GetbIsStandByState)
      (CallFunction|ScrollHandle-FinishRemainOffset false)
      (else
        (CallFunction|CheckState-ScrollHandle)))))

(fn ConstructionScript
  (|CallParentFunction)
  (CallFunction|PresetPreviewer)
  (CallFunction|PresetGeo)
  (CallFunction|PresetZoominGroup))

(fn AssignDatatoEachPreviewer
  (params (LCurrentGlass :type ST%20Glass%20Data%20Structure) (ValueSide :type E_GlassSideState%20Enum :default "NewEnumerator0"))
  (bind _output_get (LocalVariables|SetL_CurrentGlass LCurrentGlass))
  (LocalVariables|SetL_GlassValueCount_Total (Utilities|Array|Length (Utilities|Struct|BreakST_GlassData _output_get)))
  (LocalVariables|SetL_NotchSide ValueSide)
  (bind _index (Utilities|FlowControl|ForLoopwithBreak 0 7 :!label _label)
    (:LoopBody
      (if (Utilities|Enum|Equal(Enum) (Variables|/Game/Project/BluePrints/InteractOBJ/BP_GlassTotemPreviewer.BP_GlassTotemPreviewer_C|GetCurrentActivateSide (Utilities|Array|Get(acopy) (Variables|Default|GetPreviewGroup) _index)) "NewEnumerator0")
        (Default|ReceiveGLASSPreviewer :self (Utilities|Array|Get(acopy) (Variables|Default|GetPreviewGroup) _index) :ValueSide (LocalVariables|GetL_NotchSide) :CurrentGlassValue (Utilities|Array|Get(acopy) (Utilities|Struct|BreakST_GlassData LCurrentGlass) (LocalVariables|GetL_GlassValueCount)))
        (bind _output_get_2 (LocalVariables|SetL_GlassValueCount (+ (LocalVariables|GetL_GlassValueCount) 1)))
        (if (== _output_get_2 (LocalVariables|GetL_GlassValueCount_Total))
          (goto _label Break))))))

(fn AssignTotemPreviewer
  (params (CurrentGLASS :type ST%20Glass%20Data%20Structure) (NotchSide :type E_GlassSideState%20Enum :default "NewEnumerator0"))
  (LocalVariables|SetL_CurrentGlass CurrentGLASS)
  (bind _output_get (LocalVariables|SetL_NotchSide NotchSide))
  (if (Utilities|Enum|Equal(Enum) _output_get "NewEnumerator4")
    (Default|ReceiveGLASSPreviewer (Variables|Default|GetREF_GlassPreviewer) (LocalVariables|GetL_CurrentGlass) (LocalVariables|GetL_NotchSide) (Utilities|Array|Get(acopy) (Utilities|Struct|BreakST_GlassData (LocalVariables|GetL_CurrentGlass))))
    (Default|UpdateTotemRTScene (Variables|Default|GetREF_GlassManager) (Utilities|Struct|BreakST_GlassData (LocalVariables|GetL_CurrentGlass)) 1)
    (else
      (CallFunction|AssignDatatoEachPreviewer (LocalVariables|GetL_CurrentGlass) (LocalVariables|GetL_NotchSide)))))

(fn CheckState-ScrollHandle
  (if (Variables|Default|GetbIsDragScroll)
    (if (Variables|Default|GetbHasUpdateMousePivot)
      (CallFunction|ScrollHandle-DragViaInput)
      (else
        (Variables|Default|SetbHasUpdateMousePivot true)
        (CallFunction|UpdateTriggerMousePivot)))
    (else
      (Variables|Default|SetbHasUpdateMousePivot false)
      (Variables|Default|SetLatestDir_ScrollHandle 0)
      (if (<= (.z (Variables|/Script/Engine.SceneComponent|GetRelativeLocation (Variables|Default|GetScrollHandle))) -80.5)
        (if (not (Variables|Default|GetbScrollIsFinish))
          (CallFunction|ScrollHandle-FinishRemainOffset true))
        (else
          (CallFunction|ScrollHandle-FinishRemainOffset false))))))

(fn GeoCachePlayer
  (params (Percentage :type Float%20%28double-precision%29))
  (bind _output_get (LocalVariables|SetL_Percentage Percentage))
  (if (>= _output_get 1.0)
    (LocalVariables|SetL_Percentage 0.999))
  (Class|GeometryCacheComponent|SetStartTimeOffset (Variables|Default|GetScroll) (* (Variables|Default|GetGeoDuration-Scroll) (LocalVariables|GetL_Percentage))))

(fn MixGlassMerge)

(fn PresetGeo
  (Variables|Default|SetGeoDuration-Scroll (Variables|/Script/GeometryCache.GeometryCacheComponent|GetDuration (Variables|Default|GetScroll))))

(fn PresetPreviewer
  (Utilities|FlowControl|Sequence
    (:then_0
      (bind _asbp_glass_totem_previewer (Utilities|Casting|CastToBP_GlassTotemPreviewer (Variables|/Script/Engine.ChildActorComponent|GetChildActor (Variables|Default|GetCA_GlassPreview8))))
      (Utilities|Array|Add (Variables|Default|GetPreviewGroup) _asbp_glass_totem_previewer)
      (bind _asbp_glass_totem_previewer_2 (Utilities|Casting|CastToBP_GlassTotemPreviewer (Variables|/Script/Engine.ChildActorComponent|GetChildActor (Variables|Default|GetCA_GlassPreview1))))
      (Utilities|Array|Add (Variables|Default|GetPreviewGroup) _asbp_glass_totem_previewer_2))
    (:then_1
      (bind _asbp_glass_totem_previewer_3 (Utilities|Casting|CastToBP_GlassTotemPreviewer (Variables|/Script/Engine.ChildActorComponent|GetChildActor (Variables|Default|GetCA_GlassPreview2))))
      (Utilities|Array|Add (Variables|Default|GetPreviewGroup) _asbp_glass_totem_previewer_3)
      (bind _asbp_glass_totem_previewer_4 (Utilities|Casting|CastToBP_GlassTotemPreviewer (Variables|/Script/Engine.ChildActorComponent|GetChildActor (Variables|Default|GetCA_GlassPreview3))))
      (Utilities|Array|Add (Variables|Default|GetPreviewGroup) _asbp_glass_totem_previewer_4))
    (:then_2
      (bind _asbp_glass_totem_previewer_5 (Utilities|Casting|CastToBP_GlassTotemPreviewer (Variables|/Script/Engine.ChildActorComponent|GetChildActor (Variables|Default|GetCA_GlassPreview4))))
      (Utilities|Array|Add (Variables|Default|GetPreviewGroup) _asbp_glass_totem_previewer_5)
      (bind _asbp_glass_totem_previewer_6 (Utilities|Casting|CastToBP_GlassTotemPreviewer (Variables|/Script/Engine.ChildActorComponent|GetChildActor (Variables|Default|GetCA_GlassPreview5))))
      (Utilities|Array|Add (Variables|Default|GetPreviewGroup) _asbp_glass_totem_previewer_6))
    (:then_3
      (bind _asbp_glass_totem_previewer_7 (Utilities|Casting|CastToBP_GlassTotemPreviewer (Variables|/Script/Engine.ChildActorComponent|GetChildActor (Variables|Default|GetCA_GlassPreview6))))
      (Utilities|Array|Add (Variables|Default|GetPreviewGroup) _asbp_glass_totem_previewer_7)
      (bind _asbp_glass_totem_previewer_8 (Utilities|Casting|CastToBP_GlassTotemPreviewer (Variables|/Script/Engine.ChildActorComponent|GetChildActor (Variables|Default|GetCA_GlassPreview7))))
      (Utilities|Array|Add (Variables|Default|GetPreviewGroup) _asbp_glass_totem_previewer_8))
    (:then_4
      (bind _asbp_glass_totem_previewer_9 (Utilities|Casting|CastToBP_GlassTotemPreviewer (Variables|/Script/Engine.ChildActorComponent|GetChildActor (Variables|Default|GetCA_GlassPreview))))
      (Variables|Default|SetREF_GlassPreviewer _asbp_glass_totem_previewer_9))))

(fn ScrollHandle-BacktoDefault)

(fn ScrollHandle-DragViaInput
  (bind _returnvalue (Game|GetPlayerController 0))
  (bind _scrollhandle (Variables|Default|GetScrollHandle))
  (bind _triggermousepivot (Variables|Default|GetTriggerMousePivot))
  (bind _worldlocation (Game|Player|ConvertMouseLocationToWorldSpace _returnvalue))
  (bind _relativelocation (Variables|/Script/Engine.SceneComponent|GetRelativeLocation _scrollhandle))
  (bind _screenlocation (Class|PlayerController|ProjectWorldLocationtoScreen _returnvalue _worldlocation false))
  (if (!= (.y _screenlocation) (.y _triggermousepivot))
    (LocalVariables|SetL_IsFowardDir (> (.y _screenlocation) (.y _triggermousepivot)))
    (Utilities|FlowControl|Sequence
      (:then_0
        (if (LocalVariables|GetL_IsFowardDir)
          (LocalVariables|SetL_SpeedDir -1.0)
          (LocalVariables|SetL_LimitedLocation -85.5)
          (Variables|Default|SetL_CurrentDir 1)
          (else
            (LocalVariables|SetL_SpeedDir 1.0)
            (LocalVariables|SetL_LimitedLocation 2.5)
            (Variables|Default|SetL_CurrentDir -1)))
        (Variables|Default|SetbSoundPlaying (== (Variables|Default|GetL_CurrentDir) (Variables|Default|GetLatestDir_ScrollHandle)))
        (Variables|Default|SetLatestDir_ScrollHandle (Variables|Default|GetL_CurrentDir))
        (Transformation|AddLocalOffset (Variables|Default|GetScrollHandle) (Math|Vector|MakeVector 0.0 0.0 (* (Variables|Default|GetSliderSpeed) (LocalVariables|GetL_SpeedDir))) false false)
        (CallFunction|GeoCachePlayer (/ (- 2.5 (.z (Variables|/Script/Engine.SceneComponent|GetRelativeLocation (Variables|Default|GetScrollHandle)))) 88.0))
        (CallFunction|ScrollSoundEffectState true true))
      (:then_1
        (if (LocalVariables|GetL_IsFowardDir)
          (if (<= (.z (Variables|/Script/Engine.SceneComponent|GetRelativeLocation (Variables|Default|GetScrollHandle))) (LocalVariables|GetL_LimitedLocation))
            (Transformation|SetRelativeLocation _scrollhandle (Math|Vector|MakeVector (.x _relativelocation) (.y _relativelocation) (LocalVariables|GetL_LimitedLocation)) false false :!label _label)
            (Variables|Default|SetbHasUpdateMousePivot false)
            (if (== (LocalVariables|GetL_LimitedLocation) -85.5)
              (CallFunction|ScrollFinishShowPreviewer)
              (if (not (Variables|Default|GetbScrollHandleReachLimited))
                (Variables|Default|SetbScrollHandleReachLimited true)
                (Audio|SpawnSoundAttached "/Game/Project/Audio/MetaSoundSource/SE/MSS_PaperScroll_Finish.MSS_PaperScroll_Finish" (Variables|Default|GetScrollHandle) "None" "0, 0, 0" "0, 0, 0" "KeepRelativeOffset" false 1.0 1.0 0.0 0 0)
                (Variables|Default|SetbSoundPlaying false)
                (CallFunction|StopContinuedSE (Variables|Default|GetAudioEnable_ScrollHandle))
                (CallFunction|ScrollSoundEffectState false false)))
            (else
              (CallFunction|UpdateTriggerMousePivot :!label _label_2)
              (Variables|Default|SetbScrollHandleReachLimited false)
              (if (or (not (Utilities|IsValid (Variables|Default|GetAudioEnable_ScrollHandle))) (not (Variables|Default|GetbSoundPlaying)))
                (Variables|Default|SetbSoundPlaying true))))
          (elif (>= (.z (Variables|/Script/Engine.SceneComponent|GetRelativeLocation (Variables|Default|GetScrollHandle))) (LocalVariables|GetL_LimitedLocation))
            (goto _label)
            (else
              (goto _label_2))))))
    (else
      (CallFunction|ScrollSoundEffectState false true))))

(fn ScrollHandle-FinishRemainOffset
  (params (bGoingOpen :type Boolean))
  (bind _scrollhandle (Variables|Default|GetScrollHandle))
  (bind _scrollhandle_2 (Variables|Default|GetScrollHandle))
  (bind _relativelocation (Variables|/Script/Engine.SceneComponent|GetRelativeLocation _scrollhandle))
  (bind _relativelocation_2 (Variables|/Script/Engine.SceneComponent|GetRelativeLocation _scrollhandle_2))
  (bind _output_get (LocalVariables|SetL_GoingOpen bGoingOpen))
  (if _output_get
    (LocalVariables|SetL_TargetPos -85.5)
    (LocalVariables|SetL_TouchPos -84.5)
    (else
      (LocalVariables|SetL_TargetPos 2.5)
      (LocalVariables|SetL_TouchPos 1.5)))
  (Utilities|FlowControl|Sequence
    (:then_0
      (Transformation|SetRelativeLocation (Variables|Default|GetScrollHandle) (Math|Interpolation|VInterpTo (Variables|/Script/Engine.SceneComponent|GetRelativeLocation _scrollhandle_2) (Math|Vector|MakeVector (.x _relativelocation_2) (.y _relativelocation_2) (LocalVariables|GetL_TargetPos)) (Utilities|Time|GetWorldDeltaSeconds) 4.0) false false)
      (CallFunction|GeoCachePlayer (/ (- 2.5 (.z (Variables|/Script/Engine.SceneComponent|GetRelativeLocation (Variables|Default|GetScrollHandle)))) 88.0))
      (CallFunction|ScrollSoundEffectState true false))
    (:then_1
      (if (and (LocalVariables|GetL_GoingOpen) (<= (.z (Variables|/Script/Engine.SceneComponent|GetRelativeLocation (Variables|Default|GetScrollHandle))) (LocalVariables|GetL_TouchPos)))
        (CallFunction|ScrollFinishShowPreviewer)
        (Audio|SpawnSoundAttached "/Game/Project/Audio/MetaSoundSource/SE/MSS_PaperScroll_Finish.MSS_PaperScroll_Finish" (Variables|Default|GetScrollHandle) "None" "0, 0, 0" "0, 0, 0" "KeepRelativeOffset" false 1.0 1.0 0.0 0 0)
        (CallFunction|GeoCachePlayer 1.0)
        (Transformation|SetRelativeLocation _scrollhandle (Math|Vector|MakeVector (.x _relativelocation) (.y _relativelocation) (LocalVariables|GetL_TargetPos)) false false :!label _label)
        (CallFunction|ScrollSoundEffectState false false)
        (if (not (Variables|Default|GetbScrollHandleReachLimited))
          (Variables|Default|SetbScrollHandleReachLimited true)
          (Audio|SpawnSoundAttached "/Game/Project/Audio/MetaSoundSource/SE/MSS_PaperScroll_Finish.MSS_PaperScroll_Finish" (Variables|Default|GetScrollHandle) "None" "0, 0, 0" "0, 0, 0" "KeepRelativeOffset" false 1.0 1.0 0.0 0 0)
          (Variables|Default|SetbSoundPlaying false)
          (CallFunction|StopContinuedSE (Variables|Default|GetAudioEnable_ScrollHandle)))
        (elif (and (not (LocalVariables|GetL_GoingOpen)) (>= (.z (Variables|/Script/Engine.SceneComponent|GetRelativeLocation (Variables|Default|GetScrollHandle))) (LocalVariables|GetL_TouchPos)))
          (CallFunction|GeoCachePlayer 0.0)
          (goto _label))))))

(fn ScrollSoundEffectState
  (params (bIsPlaying :type Boolean) (bDragState :type Boolean))
  (LocalVariables|SetL_IsPlaying bIsPlaying)
  (if bDragState
    (if (LocalVariables|GetL_IsPlaying)
      (Variables|Default|SetScrollSE_CDtime 0.0)
      (Utilities|IsValid (Variables|Default|GetAudio_Scroll) :!label _label
        (:Is%20Valid
          (if (not (Audio|Components|Audio|IsPlaying (Variables|Default|GetAudio_Scroll)))
            (Class|AudioParameterControllerInterface|SetTriggerParameter (Variables|Default|GetAudio_Scroll) "Start")))
        (:Is%20Not%20Valid
          (bind _returnvalue (Audio|SpawnSoundAttached "/Game/Project/Audio/MetaSoundSource/SE/MSS_S1001_PaperScrollOpen.MSS_S1001_PaperScrollOpen" (Variables|Default|GetScroll) "None" "0, 0, 0" "0, 0, 0" "KeepRelativeOffset" false 1.0 1.0 0.0 0 0))
          (Variables|Default|SetAudio_Scroll _returnvalue)))
      (else
        (bind _output_get (Variables|Default|SetScrollSE_CDtime (+ (Utilities|Time|GetWorldDeltaSeconds) (Variables|Default|GetScrollSE_CDtime))))
        (if (< _output_get 0.4)
          (goto _label)
          (else
            (Utilities|IsValid (Variables|Default|GetAudio_Scroll) :!label _label_2
              (:Is%20Valid
                (Class|AudioParameterControllerInterface|SetTriggerParameter (Variables|Default|GetAudio_Scroll) "Stop")))))))
    (elif (LocalVariables|GetL_IsPlaying)
      (goto _label)
      (else
        (goto _label_2)))))

(fn UpdateTotemPreviewer)

(fn UpdateTriggerMousePivot
  (bind _returnvalue (Game|GetPlayerController 0))
  (Variables|Default|SetTriggerMousePivot (.ScreenLocation (Class|PlayerController|ProjectWorldLocationtoScreen _returnvalue (.WorldLocation (Game|Player|ConvertMouseLocationToWorldSpace _returnvalue)) false))))

(fn PresetZoominGroup
  (Utilities|Array|Add (Variables|Default|GetWidgetTriggerGroup) (Variables|Default|GetWidgetTrigger_Main)))

(fn SwitchMeshCollisionProfile
  (params (bIsBlock :type Boolean))
  (if bIsBlock
    (LocalVariables|SetL_ProfileName "StandByMode")
    (else
      (LocalVariables|SetL_ProfileName "NoCollision")))
  (Collision|SetCollisionProfileName (Variables|Default|GetScrollHandle) (LocalVariables|GetL_ProfileName) true :!class /Script/Engine.PrimitiveComponent))

(fn ScrollFinishShowPreviewer
  (Variables|Default|SetbScrollIsFinish true)
  (Transformation|SetRelativeLocation (Variables|Default|GetGlassPreview_Mix) "0, 0, 0" false false))