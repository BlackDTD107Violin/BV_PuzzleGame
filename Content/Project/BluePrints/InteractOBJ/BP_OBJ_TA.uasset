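; BP_OBJ_TA is an interaction trigger area that manages placing and removing puzzle items in machine notches.
; It configures itself as Key, Extract or Glass from the notch type and links to its parent stand or BP_S9007 notch.
; Insertions spawn the item through the notch, play a sound and route data to the extract, main or final machine by side.
; Pick-outs restore collision and clear notch state.
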(fn ConstructionScript)

(fn RefreshInsertedOBJ
  (params (InsertedOBJ :type ST%20Item%20Collection%20Structure))
  (Variables|Default|SetInsertedOBJ InsertedOBJ)
  (Default|ReceiveOBJExtractCode (Variables|/Game/Project/BluePrints/InteractOBJ/BP_S9007.BP_S9007_C|GetREF_Extract%20Machine (Variables|Default|GetREF_OBJnotch)) (Variables|Default|GetInsertedOBJ))
  (Default|SpawnOBJActor (Variables|Default|GetREF_OBJnotch) (.TargetItemActor (Utilities|Struct|BreakST_ItemCollection (Variables|Default|GetInsertedOBJ))))
  (Rendering|SetActorHiddenInGame (.TargetItemActor (Utilities|Struct|BreakST_ItemCollection (Variables|Default|GetInsertedOBJ))) false)
  (Collision|SetActorEnableCollision (.TargetItemActor (Utilities|Struct|BreakST_ItemCollection (Variables|Default|GetInsertedOBJ))) true)
  (Audio|SpawnSoundAttached (.PlaceSE (Utilities|Struct|BreakST_ItemCollection (Variables|Default|GetInsertedOBJ))) (Variables|Default|GetKey_TriggerArea) "None" "0, 0, 0" "0, 0, 0" "KeepRelativeOffset" false 1.0 1.0 0.0 0 0)
  (Variables|Default|SetbExtractTAIsEmpty false)
  (bind _asbp_core_item_key (Utilities|Casting|CastToBP_CoreITEM_KEY (Utilities|Struct|BreakST_ItemCollection (Variables|Default|GetInsertedOBJ)))
    (:then
      (Variables|/Game/Project/Core/InteractOBJ/BP_CoreITEM_KEY.BP_CoreITEM_KEY_C|SetCurrentInsertedExtractTA _asbp_core_item_key self))
    (:CastFailed
      (bind _asbp_core_item_extract (Utilities|Casting|CastToBP_CoreITEM_EXTRACT (Utilities|Struct|BreakST_ItemCollection (Variables|Default|GetInsertedOBJ)))))))

(fn RefreshInsertedGLASS
  (params (InsertedGlass :type ST%20Glass%20Data%20Structure))
  (bind _ref_glassnotch (Variables|Default|GetREF%20GlassNotch))
  (bind _ref_finalmachine (Variables|/Game/Project/BluePrints/InteractOBJ/BP_S9007.BP_S9007_C|GetREF_FinalMachine _ref_glassnotch))
  (Variables|Default|SetInsertedGlass InsertedGlass)
  (Utilities|FlowControl|Sequence
    (:then_0
      (LocalVariables|SetL_GlassValues (Utilities|Struct|BreakST_GlassData (Variables|Default|GetInsertedGlass)))
      (Audio|SpawnSoundAttached "/Game/Project/Audio/MetaSoundSource/SE/MSS_Pick_Place_Metal_5.MSS_Pick_Place_Metal_5" (Variables|Default|GetKey_TriggerArea) "None" "0, 0, 0" "0, 0, 0" "KeepRelativeOffset" false 1.0 1.0 0.0 0 0))
    (:then_1
      (switch Utilities|FlowControl|Switch|SwitchonE_GlassSideState (Variables|Default|GetGlassTAside)
        (:NewEnumerator1
          (Variables|/Game/Project/BluePrints/InteractOBJ/BP_S9001.BP_S9001_C|SetLeftInsertedGlass (Variables|/Game/Project/BluePrints/InteractOBJ/BP_S9007.BP_S9007_C|GetREF_MainMachine (Variables|Default|GetREF%20GlassNotch)) (Variables|Default|GetInsertedGlass))
          (Variables|Default|SetSideIndex 2))
        (:NewEnumerator2
          (Variables|/Game/Project/BluePrints/InteractOBJ/BP_S9001.BP_S9001_C|SetRightInsertedGlass (Variables|/Game/Project/BluePrints/InteractOBJ/BP_S9007.BP_S9007_C|GetREF_MainMachine (Variables|Default|GetREF%20GlassNotch)) (Variables|Default|GetInsertedGlass))
          (Variables|Default|SetSideIndex 3))
        (:NewEnumerator4
          (Variables|/Game/Project/BluePrints/InteractOBJ/BP_S9001.BP_S9001_C|SetDownInsertedGlass (Variables|/Game/Project/BluePrints/InteractOBJ/BP_S9007.BP_S9007_C|GetREF_MainMachine (Variables|Default|GetREF%20GlassNotch)) (Variables|Default|GetInsertedGlass))
          (Variables|Default|SetSideIndex 1)
          (Variables|/Game/Project/BluePrints/InteractOBJ/BP_S9001.BP_S9001_C|SetDownInsertedGlassValue (Variables|/Game/Project/BluePrints/InteractOBJ/BP_S9007.BP_S9007_C|GetREF_MainMachine (Variables|Default|GetREF%20GlassNotch)) (Utilities|Array|Get(acopy) (LocalVariables|GetL_GlassValues))))
        (:NewEnumerator6
          (Variables|/Game/Project/BluePrints/InteractOBJ/BP_S9009.BP_S9009_C|SetInsertedGlass _ref_finalmachine (Variables|Default|GetInsertedGlass))
          (Variables|Default|SetSideIndex 4)
          (Default|CertifyStartCheckMatchCode _ref_finalmachine)))
      (Default|SpawnGlassActor (Variables|Default|GetREF%20GlassNotch) (Variables|Default|GetSideIndex) (Utilities|Struct|BreakST_GlassData (Variables|Default|GetInsertedGlass))))))

(fn SetupNewGlass
  (params (Glass%20Data :type BP%20Core%20ITEM%20GLASS%20Object%20Reference) (SideIndex :type Integer))
  (LocalVariables|SetL_GlassData Glass%20Data)
  (Default|SpawnGlassActor (Variables|Default|GetREF%20GlassNotch) SideIndex (LocalVariables|GetL_GlassData)))

(fn ResetAfterMerge
  (Collision|SetCollisionEnabled (Variables|Default|GetKey_TriggerArea) "QueryAndPhysics")
  (Variables|Default|SetbThisTAIsEmpty true))

(fn PickOutGlass
  (bind _ref_glassnotch (Variables|Default|GetREF%20GlassNotch))
  (bind _ref_glassnotch_2 (Variables|Default|GetREF%20GlassNotch))
  (bind _ref_extract_machine (Variables|/Game/Project/BluePrints/InteractOBJ/BP_S9007.BP_S9007_C|GetREF_Extract%20Machine _ref_glassnotch))
  (Utilities|FlowControl|Sequence
    (:then_0
      (Variables|Default|SetbThisTAIsEmpty true)
      (Collision|SetCollisionEnabled (Variables|Default|GetKey_TriggerArea) "QueryAndPhysics")
      (Variables|/Game/Project/Core/InteractOBJ/BP_CoreITEM.BP_CoreITEM_C|SetbCanTake (Variables|/Game/Project/BluePrints/InteractOBJ/BP_S9007.BP_S9007_C|GetREF_InsertedGLASS _ref_glassnotch_2) false)
      (Utilities|Array|Clear (Variables|/Game/Project/Core/InteractOBJ/BP_CoreSTAND.BP_CoreSTAND_C|GetChildLists _ref_glassnotch_2)))
    (:then_1
      (Utilities|IsValid (Variables|/Game/Project/BluePrints/InteractOBJ/BP_S9007.BP_S9007_C|GetREF_Extract%20Machine (Variables|Default|GetREF%20GlassNotch))
        (:Is%20Valid
          (Variables|/Game/Project/BluePrints/InteractOBJ/BP_S9008.BP_S9008_C|SetbResultIsEmpty _ref_extract_machine true)
          (Default|CheckState-DiamondCurrent _ref_extract_machine))
        (:Is%20Not%20Valid
          _))
      (return (Variables|Default|GetGlassTAside)))))

(fn PickOutOBJ
  (bind _ref_objnotch (Variables|Default|GetREF_OBJnotch))
  (Variables|Default|SetbExtractTAIsEmpty true)
  (Collision|SetCollisionEnabled (Variables|Default|GetKey_TriggerArea) "QueryAndPhysics")
  (Utilities|Array|Clear (Variables|/Game/Project/Core/InteractOBJ/BP_CoreSTAND.BP_CoreSTAND_C|GetChildLists _ref_objnotch))
  (Variables|/Game/Project/BluePrints/InteractOBJ/BP_S9008.BP_S9008_C|SetbOBJIsSet (Variables|/Game/Project/BluePrints/InteractOBJ/BP_S9007.BP_S9007_C|GetREF_Extract%20Machine _ref_objnotch) false)
  (return (Variables|Default|GetGlassTAside)))

(fn UpdateTotemandPanel
  (if (not (Variables|Default|GetbThisTAIsEmpty))
    (Default|ReceiveGLASSCode (Variables|/Game/Project/BluePrints/InteractOBJ/BP_S9007.BP_S9007_C|GetREF_MainMachine (Variables|Default|GetREF%20GlassNotch)) (Variables|Default|GetInsertedGlass))))

(fn PresetNotchValue
  (params (GlassNotchType :type E_GlassSideState%20Enum :default "NewEnumerator0"))
  (switch Utilities|FlowControl|Switch|SwitchonE_GlassSideState GlassNotchType
    (:NewEnumerator0
      (Variables|Default|SetThisTAType "NewEnumerator0"))
    (:NewEnumerator1
      (Variables|Default|SetThisTAType "NewEnumerator2" :!label _label))
    (:NewEnumerator2
      (goto _label))
    (:NewEnumerator3
      (goto _label))
    (:NewEnumerator4
      (goto _label))
    (:NewEnumerator5
      (Variables|Default|SetThisTAType "NewEnumerator1"))
    (:NewEnumerator6
      (goto _label)))
  (switch Utilities|FlowControl|Switch|SwitchonE_TAType (Variables|Default|GetThisTAType)
    (:NewEnumerator0
      (bind _asbp_core_stand_set (Utilities|Casting|CastToBP_CoreSTAND_SET (Actor|GetParentActor)))
      (Variables|Default|SetParentActor _asbp_core_stand_set))
    (:NewEnumerator1
      (bind _asbp_s9007 (Utilities|Casting|CastToBP_S9007 (Actor|GetParentActor)))
      (Variables|Default|SetREF_OBJnotch _asbp_s9007))
    (:NewEnumerator2
      (bind _asbp_s9007_2 (Utilities|Casting|CastToBP_S9007 (Actor|GetParentActor)))
      (bind _output_get (Variables|Default|SetREF%20GlassNotch _asbp_s9007_2))
      (Variables|Default|SetGlassTAside (Variables|/Game/Project/BluePrints/InteractOBJ/BP_S9007.BP_S9007_C|GetGlassNotchType _output_get)))))