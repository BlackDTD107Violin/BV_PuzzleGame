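; BP_S0002 is an interactable stand with a lockable door that the tutorial player inspects in a zoomed view.
; Zoomin blends the camera to the actor, blocks player input, disables its trigger and shows a one-time door-trick tutorial.
; ZoomOut restores view and input, re-enabling the trigger only while still locked.
; InteractiveUnlocked flip-flops a door timeline between open and reversed close, clearing the lock and playing a sound on opening.
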(event Custom|AnimPlay_CloseDoor
  ;[0.05098 0.05098 0.05098] Door Animation
  (bind _doortrack (Timeline|Timeline Reverse)
    (:Update
      (Transformation|SetRelativeRotation (Variables|Default|GetSM_Door) (Math|Rotator|MakeRotator _doortrack 9e+01 0.0) false false))))

(event Custom|AnimPlay_OpenDoor
  ;[0.05098 0.05098 0.05098] Door Animation
  (bind _doortrack (Timeline|Timeline Play)
    (:Update
      (Transformation|SetRelativeRotation (Variables|Default|GetSM_Door) (Math|Rotator|MakeRotator _doortrack 9e+01 0.0) false false))))

(event EventBeginPlay
  (|CallParentFunction)
  (bind _asbp_first_person_character_tutorial (Utilities|Casting|CastToBP_FirstPersonCharacterTutorial (Game|GetPlayerCharacter 0)))
  (Variables|Default|SetPlayer_Tutorial _asbp_first_person_character_tutorial))

(event EventInteractiveUnlocked
  (params (MatchOBJCode :type Name :default "None"))
  ;[0.05098 0.05098 0.05098] CheckUnlockState
  (Utilities|FlowControl|Delay 0.2)
  (Utilities|FlowControl|FlipFlop
    (:A
      (CallFunction|AnimPlayOpenDoor)
      (Variables|Default|SetbSTANDIsLocked false)
      (Audio|SpawnSoundatLocation "/Game/Project/Audio/MetaSoundSource/SE/MSS_S0002_OpenDoor.MSS_S0002_OpenDoor" (Transformation|GetWorldLocation (Variables|Default|GetStaticMesh)) "0, 0, 0" 1.0 1.0 0.0 0 0))
    (:B
      (CallFunction|AnimPlayCloseDoor))))

(event EventZoomin
  (params (ZoomComponent :type Actor%20Component%20Object%20Reference))
  (bind _returnvalue (Game|GetPlayerController 0))
  (bind _player_tutorial (Variables|Default|GetPlayer_Tutorial))
  (Utilities|FlowControl|Sequence
    (:then_0
      (Game|Player|SetViewTargetwithBlend (Game|GetPlayerController 0) self 0.5 "VTBlend_Linear" 0.0 true)
      (Input|SetIgnoreMoveInput _returnvalue true)
      (Input|SetIgnoreLookInput _returnvalue true)
      (Default|ClearGamePromptUIView (Variables|Default|GetPlayer_Tutorial))
      (Collision|SetCollisionProfileName (Variables|Default|GetZoomTrigger_Main) "NoCollision" true :!class /Script/Engine.PrimitiveComponent))
    (:then_1
      (if (not (Variables|Default|GetbHasTriggerTutor))
        (Variables|Default|SetbHasTriggerTutor true)
        (Utilities|FlowControl|Delay 0.5)
        (Default|EnterDoorTRICK _player_tutorial)
        (Default|ClearGamePromptUIView _player_tutorial)))))

(event EventZoomOut
  (bind _returnvalue (Game|GetPlayerController 0))
  (Game|Player|SetViewTargetwithBlend (Game|GetPlayerController 0) (Game|GetPlayerCharacter 0) 0.5 "VTBlend_Linear" 0.0 true)
  (Input|ResetIgnoreMoveInput _returnvalue)
  (Input|ResetIgnoreLookInput _returnvalue)
  (Utilities|FlowControl|Delay 0.5)
  (if (Variables|Default|GetbSTANDIsLocked)
    (Collision|SetCollisionProfileName (Variables|Default|GetZoomTrigger_Main) "StandByMode" true :!class /Script/Engine.PrimitiveComponent)))

(fn ConstructionScript
  (|CallParentFunction))