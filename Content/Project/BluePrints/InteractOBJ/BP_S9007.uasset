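; BP_S9007 is a zoomable placement slot for glass slides and extractable items, identifying its parent as the Main (S9001), Extract (S9008) or Final (S9009) machine.
; Its child BP_OBJ_TA trigger receives pooled glass built from extract or mix data, with collision toggled by slot occupancy.
; Placed glass gets a render-target totem material and registers with the machine.
; A timeline floats and rotates extract items using their component's settings.
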(event Custom|Film_ExtractFloating
  (bind _placelocation (Variables|Default|GetPlaceLocation))
  (bind _returnvalue (Transformation|GetWorldLocation _placelocation))
  (Variables|Default|SetBaseAngle (Transformation|GetActorRotation (Variables|Default|GetREF_InsertedOBJ)))
  (Utilities|IsValid (Variables|Default|GetREF_InsertedOBJ)
    (:Is%20Valid
      (bind (_direction _floatheight _floatangle) (Timeline|OBJFloating PlayFromStart)
        (:Update
          (Transformation|SetActorLocation (Variables|Default|GetREF_InsertedOBJ) (Math|Vector|MakeVector (.x _returnvalue) (.y _returnvalue) (Math|Float|Lerp (.z _returnvalue) (+ (.z _returnvalue) (Variables|Default|GetFloatHeight)) _floatheight)) false false)
          (Transformation|SetActorRotation (Variables|Default|GetREF_InsertedOBJ) (Math|Rotator|Lerp(Rotator) (Variables|Default|GetBaseAngle) (Variables|Default|GetFloat%20Angle) _floatangle)))
        (:SEPlay
          (bind _asbp_core_item_extract (Utilities|Casting|CastToBP_CoreITEM_EXTRACT (Variables|Default|GetREF_InsertedOBJ)))
          (Audio|SpawnSoundAttached (Variables|/Game/Project/Core/InteractOBJ/AC_ExtractComponent.AC_ExtractComponent_C|GetExtractDropSE (Variables|/Game/Project/Core/InteractOBJ/BP_CoreITEM_EXTRACT.BP_CoreITEM_EXTRACT_C|GetAC_ExtractComponent _asbp_core_item_extract)) (Variables|Default|GetPlaceLocation) "None" "0, 0, 0" "0, 0, 0" "KeepRelativeOffset" false 1.0 1.0 0.0 0 0))))))

(event EventBeginPlay
  (|CallParentFunction))

(event EventZoomin
  (params (ZoomComponent :type Actor%20Component%20Object%20Reference))
  (|CallParentFunction ZoomComponent)
  (if (> (Utilities|Array|Length (Variables|Default|GetChildLists)) 0)
    (CallFunction|SwitchMeshCollisionProfile false)
    (else
      (CallFunction|SwitchMeshCollisionProfile true))))

(event EventZoomOut
  (|CallParentFunction))

(fn ConstructionScript
  (|CallParentFunction)
  (CallFunction|PresetValue)
  (CallFunction|PresetZoominGroup))

(fn AcquireGlassfromPool
  (bind _ref_glassmanager (Variables|Default|GetREF_GlassManager))
  (bind _glasspool (Variables|/Game/Project/Core/GameSystem/BP_GlassManager.BP_GlassManager_C|GetGlassPool _ref_glassmanager))
  (bind _returnvalue (Utilities|Array|Length _glasspool))
  (if (> _returnvalue 0)
    (Variables|Default|SetMaxPool _returnvalue)
    (Utilities|IsValid (Utilities|Array|Get(acopy) _glasspool (Variables|Default|GetGlassIndex))
      (:Is%20Valid
        (bind _result (Math|Integer|IncrementInt (Variables|Default|GetGlassIndex))
          (:%20%20
            (bind _output_get (Variables|Default|SetGlassIndex _result))
            (if (== _output_get (Variables|Default|GetMaxPool))
              (Variables|Default|SetGlassIndex 0))
            (return (Utilities|Array|Get(acopy) _glasspool (Variables|Default|GetGlassIndex))))))
      (:Is%20Not%20Valid
        _)))
  (return 0))

(fn CollisionbyAutoState
  (params (bIsOpen :type Boolean))
  (if bIsOpen
    (if (> (Utilities|Array|Length (Variables|Default|GetChildLists)) 0)
      (CallFunction|SwitchMeshCollisionProfile false)
      (for _array_element (Variables|Default|GetChildLists)
        (Collision|SetCollisionProfileName (Variables|/Game/Project/Core/InteractOBJ/BP_CoreOBJ.BP_CoreOBJ_C|GetStaticMesh _array_element) "StandByMode" true :!class /Script/Engine.PrimitiveComponent))
      (else
        (CallFunction|SwitchMeshCollisionProfile true)))
    (else
      (CallFunction|SwitchMeshCollisionProfile true))))

(fn PlaceLocationOffset
  (params (NewParam :type Vector))
  (Transformation|SetRelativeLocation (Variables|Default|GetPlaceLocation) (+ NewParam (Variables|/Script/Engine.SceneComponent|GetRelativeLocation (Variables|Default|GetPlaceLocation))) false false))

(fn PresetValue
  (bind _returnvalue (Actor|GetParentActor))
  (Utilities|FlowControl|Sequence
    (:then_0
      (bind _asbp_obj_ta (Utilities|Casting|CastToBP_OBJ_TA (Variables|/Script/Engine.ChildActorComponent|GetChildActor (Variables|Default|GetGLASS_TA))))
      (bind _output_get (Variables|Default|SetREF_OBJ%20TA _asbp_obj_ta))
      (Default|PresetNotchValue _output_get (Variables|Default|GetGlassNotchType))
      (CallFunction|SwitchMeshCollisionProfile true))
    (:then_1
      (Utilities|IsValid _returnvalue
        (:Is%20Valid
          (bind _asbp_s9001 (Utilities|Casting|CastToBP_S9001 _returnvalue)
            (:then
              (Variables|Default|SetREF_MainMachine _asbp_s9001)
              (Variables|Default|SetGlassMachineType "NewEnumerator0"))
            (:CastFailed
              (bind _asbp_s9008 (Utilities|Casting|CastToBP_S9008 (Actor|GetParentActor))
                (:then
                  (Variables|Default|SetREF_Extract%20Machine _asbp_s9008)
                  (Variables|Default|SetGlassMachineType "NewEnumerator1"))
                (:CastFailed
                  (bind _asbp_s9009 (Utilities|Casting|CastToBP_S9009 (Actor|GetParentActor)))
                  (Variables|Default|SetREF_FinalMachine _asbp_s9009)
                  (Variables|Default|SetGlassMachineType "NewEnumerator2"))))))))))

(fn RemoveGlassTAside
  (params (Side :type E_GlassSideState%20Enum :default "NewEnumerator0"))
  (Default|EraseTotemPreviewer (Variables|Default|GetREF_MainMachine) Side))

(fn ReturnGlassTAside
  (bind _asbp_obj_ta (Utilities|Casting|CastToBP_OBJ_TA (Variables|/Script/Engine.ChildActorComponent|GetChildActor (Variables|Default|GetGLASS_TA))))
  (return (Variables|/Game/Project/BluePrints/InteractOBJ/BP_OBJ_TA.BP_OBJ_TA_C|GetGlassTAside _asbp_obj_ta)))

(fn ReceiveExtractDataandCreate
  (params (Data :type ST%20Glass%20Value%20Structure))
  (Variables|Default|SetCurrentExtractData Data)
  (Utilities|FlowControl|Sequence
    (:then_0
      (bind _glassfrompool (Default|AcquireGlassfromPool (Variables|Default|GetREF_GlassManager)))
      (bind _output_get (LocalVariables|SetL_Temp_GLASSbase _glassfrompool))
      (Transformation|SetActorTransform _output_get (Math|Conversions|ToTransform(Vector) (Transformation|GetWorldLocation (Variables|Default|GetPlaceLocation))))
      (Variables|/Game/Project/BluePrints/InteractOBJ/BP_GLASSItem.BP_GLASSItem_C|SetThisGlass (LocalVariables|GetL_Temp_GLASSbase) (Utilities|Struct|MakeST_GlassData (LocalVariables|GetL_Temp_GLASSbase) -1 0 (Utilities|Array|MakeArray (Variables|Default|GetCurrentExtractData)) 0 0))
      (bind _previewmat (Default|ReturnRenderMatScene (Variables|/Game/Project/BluePrints/InteractOBJ/BP_GLASSItem.BP_GLASSItem_C|GetREF_GlassManager (LocalVariables|GetL_Temp_GLASSbase))))
      (Rendering|Material|SetMaterial (Variables|/Game/Project/Core/InteractOBJ/BP_CoreOBJ.BP_CoreOBJ_C|GetStaticMesh (LocalVariables|GetL_Temp_GLASSbase)) 3 _previewmat)
      (Default|SwitchStateRenderMatScene (Variables|/Game/Project/BluePrints/InteractOBJ/BP_GLASSItem.BP_GLASSItem_C|GetREF_GlassManager (LocalVariables|GetL_Temp_GLASSbase)) 0 true))
    (:then_1
      (bind _asbp_obj_ta (Utilities|Casting|CastToBP_OBJ_TA (Variables|/Script/Engine.ChildActorComponent|GetChildActor (Variables|Default|GetGLASS_TA))))
      (Default|SetupNewGlass _asbp_obj_ta (LocalVariables|GetL_Temp_GLASSbase))
      (Collision|SetCollisionEnabled (Variables|/Game/Project/BluePrints/InteractOBJ/BP_OBJ_TA.BP_OBJ_TA_C|GetKey_TriggerArea _asbp_obj_ta) "NoCollision")
      (Collision|SetCollisionEnabled (Variables|/Game/Project/Core/InteractOBJ/BP_CoreOBJ.BP_CoreOBJ_C|GetStaticMesh (Utilities|Array|Get(acopy) (Variables|Default|GetChildLists))) "NoCollision"))))

(fn ReceiveMixDataandCreate
  (params (GlassUnite :type ST%20Glass%20Data%20Structure))
  (Variables|Default|SetCurrentGLASS GlassUnite)
  (Utilities|FlowControl|Sequence
    (:then_0
      (bind _glassfrompool (Default|AcquireGlassfromPool (Variables|Default|GetREF_GlassManager)))
      (bind _output_get (LocalVariables|SetL_Temp_GLASSbase _glassfrompool))
      (Transformation|SetActorTransform _output_get (Math|Conversions|ToTransform(Vector) (Transformation|GetWorldLocation (Variables|Default|GetPlaceLocation))))
      (Variables|/Game/Project/BluePrints/InteractOBJ/BP_GLASSItem.BP_GLASSItem_C|SetThisGlass (LocalVariables|GetL_Temp_GLASSbase) (Utilities|Struct|MakeST_GlassData (LocalVariables|GetL_Temp_GLASSbase) -1 (.inheritlayer (Variables|Default|GetCurrentGLASS)) (.glassvalue (Variables|Default|GetCurrentGLASS)) 0 0))
      (Variables|/Game/Project/Core/InteractOBJ/BP_CoreITEM_GLASS.BP_CoreITEM_GLASS_C|SetGlassType (LocalVariables|GetL_Temp_GLASSbase) "NewEnumerator1")
      (switch int (.inheritlayer (Variables|Default|GetCurrentGLASS))
        (:1
          (Variables|/Game/Project/Core/InteractOBJ/BP_CoreOBJ.BP_CoreOBJ_C|SetOBJSerialCode (LocalVariables|GetL_Temp_GLASSbase) "G_Unite1"))
        (:2
          (Variables|/Game/Project/Core/InteractOBJ/BP_CoreOBJ.BP_CoreOBJ_C|SetOBJSerialCode (LocalVariables|GetL_Temp_GLASSbase) "G_Unite2"))
        (:3
          (Variables|/Game/Project/Core/InteractOBJ/BP_CoreOBJ.BP_CoreOBJ_C|SetOBJSerialCode (LocalVariables|GetL_Temp_GLASSbase) "G_Unite3"))))
    (:then_1
      (bind _asbp_obj_ta (Utilities|Casting|CastToBP_OBJ_TA (Variables|/Script/Engine.ChildActorComponent|GetChildActor (Variables|Default|GetGLASS_TA))))
      (Default|SetupNewGlass _asbp_obj_ta (LocalVariables|GetL_Temp_GLASSbase) 4)
      (Collision|SetCollisionEnabled (Variables|/Game/Project/BluePrints/InteractOBJ/BP_OBJ_TA.BP_OBJ_TA_C|GetKey_TriggerArea _asbp_obj_ta) "NoCollision")
      (Collision|SetCollisionEnabled (Variables|/Game/Project/Core/InteractOBJ/BP_CoreOBJ.BP_CoreOBJ_C|GetStaticMesh (Utilities|Array|Get(acopy) (Variables|Default|GetChildLists))) "NoCollision"))))

(fn SetupGlassTAside
  (params (GlassTAside :type E_GlassSideState%20Enum :default "NewEnumerator0"))
  (bind _asbp_obj_ta (Utilities|Casting|CastToBP_OBJ_TA (Variables|/Script/Engine.ChildActorComponent|GetChildActor (Variables|Default|GetGLASS_TA))))
  (Variables|/Game/Project/BluePrints/InteractOBJ/BP_OBJ_TA.BP_OBJ_TA_C|SetGlassTAside _asbp_obj_ta GlassTAside))

(fn SpawnGlassActor
  (params (SideIndex :type Integer) (GlassData :type BP%20Core%20ITEM%20GLASS%20Object%20Reference))
  (LocalVariables|SetL_SideIndex SideIndex)
  (bind _asbp_glassitem (Utilities|Casting|CastToBP_GLASSItem GlassData))
  (bind _output_get (Variables|Default|SetREF_InsertedGLASS _asbp_glassitem))
  (Variables|/Game/Project/Core/InteractOBJ/BP_CoreITEM.BP_CoreITEM_C|SetbCanTake _output_get true)
  (Utilities|FlowControl|Sequence
    (:then_0
      (LocalVariables|SetL_GlassValue (.glassvalue (Variables|/Game/Project/BluePrints/InteractOBJ/BP_GLASSItem.BP_GLASSItem_C|GetThisGlass (Variables|Default|GetREF_InsertedGLASS))))
      (if (Utilities|Enum|Equal(Enum) (Variables|/Game/Project/Core/InteractOBJ/BP_CoreITEM_GLASS.BP_CoreITEM_GLASS_C|GetGlassType (Variables|Default|GetREF_InsertedGLASS)) "NewEnumerator6")
        (Components|StaticMesh|SetStaticMesh (Variables|/Game/Project/Core/InteractOBJ/BP_CoreOBJ.BP_CoreOBJ_C|GetStaticMesh (Variables|Default|GetREF_InsertedGLASS)) "/Game/Project/Artist/KeyObj/Mesh/SM_Slider_Single.SM_Slider_Single")
        (else
          (Components|StaticMesh|SetStaticMesh (Variables|/Game/Project/Core/InteractOBJ/BP_CoreOBJ.BP_CoreOBJ_C|GetStaticMesh (Variables|Default|GetREF_InsertedGLASS)) "/Game/Project/Artist/KeyObj/Mesh/SM_Slider_Combine.SM_Slider_Combine")
          (Default|SetInheritDiamond (Variables|Default|GetREF_InsertedGLASS)))))
    (:then_1
      (Default|UpdateTotemRTScene (Variables|/Game/Project/BluePrints/InteractOBJ/BP_GLASSItem.BP_GLASSItem_C|GetREF_GlassManager (Variables|Default|GetREF_InsertedGLASS)) (LocalVariables|GetL_GlassValue) (LocalVariables|GetL_SideIndex))
      (bind _previewmat (Default|ReturnRenderMatScene (Variables|/Game/Project/BluePrints/InteractOBJ/BP_GLASSItem.BP_GLASSItem_C|GetREF_GlassManager (Variables|Default|GetREF_InsertedGLASS)) (LocalVariables|GetL_SideIndex)))
      (Rendering|Material|SetMaterial (Variables|/Game/Project/Core/InteractOBJ/BP_CoreOBJ.BP_CoreOBJ_C|GetStaticMesh (Variables|Default|GetREF_InsertedGLASS)) 3 _previewmat))
    (:then_2
      (Development|SetHiddeninGame (Variables|/Game/Project/Core/InteractOBJ/BP_CoreOBJ.BP_CoreOBJ_C|GetStaticMesh (Variables|Default|GetREF_InsertedGLASS)) false false)
      (Transformation|SetActorLocation (Variables|Default|GetREF_InsertedGLASS) (Transformation|GetWorldLocation (Variables|Default|GetPlaceLocation)) false false)
      (Transformation|AttachActorToActor (Variables|Default|GetREF_InsertedGLASS) self "None" "KeepWorld" "KeepRelative" "KeepRelative" true))
    (:then_3
      (Transformation|SetActorRelativeRotation (Variables|Default|GetREF_InsertedGLASS) "0.000000,90.000000,0.000000")
      (Transformation|SetWorldScale3D (Variables|/Game/Project/Core/InteractOBJ/BP_CoreOBJ.BP_CoreOBJ_C|GetStaticMesh (Variables|Default|GetREF_InsertedGLASS)) "1.000000,1.000000,1.000000")
      (Utilities|Array|Add (Variables|Default|GetChildLists) (Variables|Default|GetREF_InsertedGLASS))
      (switch Utilities|FlowControl|Switch|SwitchonE_GlassMachine (Variables|Default|GetGlassMachineType)
        (:NewEnumerator0
          (Utilities|Array|Add (Variables|/Game/Project/Core/InteractOBJ/BP_CoreSTAND_SET.BP_CoreSTAND_SET_C|GetChildLists (Variables|Default|GetREF_MainMachine)) (Variables|Default|GetREF_InsertedGLASS)))
        (:NewEnumerator1
          (Utilities|Array|Add (Variables|/Game/Project/Core/InteractOBJ/BP_CoreSTAND_SET.BP_CoreSTAND_SET_C|GetChildLists (Variables|Default|GetREF_Extract%20Machine)) (Variables|Default|GetREF_InsertedGLASS)))
        (:NewEnumerator2
          (Utilities|Array|Add (Variables|/Game/Project/Core/InteractOBJ/BP_CoreSTAND_SET.BP_CoreSTAND_SET_C|GetChildLists (Variables|Default|GetREF_FinalMachine)) (Variables|Default|GetREF_InsertedGLASS)))))))

(fn SpawnOBJActor
  (params (InteractTarget :type Actor%20Object%20Reference))
  (bind _asbp_core_item (Utilities|Casting|CastToBP_CoreITEM InteractTarget))
  (bind _output_get (Variables|Default|SetREF_InsertedOBJ _asbp_core_item))
  (Development|SetHiddeninGame (Variables|/Game/Project/Core/InteractOBJ/BP_CoreOBJ.BP_CoreOBJ_C|GetStaticMesh _output_get) false false)
  (Utilities|FlowControl|Sequence
    (:then_0
      (Transformation|SetActorLocation (Variables|Default|GetREF_InsertedOBJ) (Transformation|GetWorldLocation (Variables|Default|GetPlaceLocation)) false false))
    (:then_1
      (bind _asbp_core_item_extract (Utilities|Casting|CastToBP_CoreITEM_EXTRACT (Variables|Default|GetREF_InsertedOBJ)))
      (Variables|Default|SetFloatHeight (Variables|/Game/Project/Core/InteractOBJ/AC_ExtractComponent.AC_ExtractComponent_C|GetExtractFloatHeight (Variables|/Game/Project/Core/InteractOBJ/BP_CoreITEM_EXTRACT.BP_CoreITEM_EXTRACT_C|GetAC_ExtractComponent _asbp_core_item_extract)))
      (Variables|Default|SetFloat%20Angle (Variables|/Game/Project/Core/InteractOBJ/AC_ExtractComponent.AC_ExtractComponent_C|GetExtractFloatAngle (Variables|/Game/Project/Core/InteractOBJ/BP_CoreITEM_EXTRACT.BP_CoreITEM_EXTRACT_C|GetAC_ExtractComponent _asbp_core_item_extract))))
    (:then_2
      (Utilities|Array|Add (Variables|Default|GetChildLists) (Variables|Default|GetREF_InsertedOBJ))
      (Utilities|Array|Add (Variables|/Game/Project/Core/InteractOBJ/BP_CoreSTAND_SET.BP_CoreSTAND_SET_C|GetChildLists (Variables|Default|GetREF_Extract%20Machine)) (Variables|Default|GetREF_InsertedOBJ)))))

(fn UpdateGLASSCode
  (bind _ref_insertedglass (Variables|Default|GetREF_InsertedGLASS))
  (bind _updatedglass (Default|ReturnUpdatedGLASSCode (Variables|Default|GetREF_MainMachine) (Variables|Default|GetGlassNotchType)))
  (Variables|/Game/Project/BluePrints/InteractOBJ/BP_GLASSItem.BP_GLASSItem_C|SetThisGlass (Variables|Default|GetREF_InsertedGLASS) _updatedglass)
  (bind _previewmat (Default|ReturnRenderMatScene (Variables|/Game/Project/BluePrints/InteractOBJ/BP_GLASSItem.BP_GLASSItem_C|GetREF_GlassManager _ref_insertedglass) 1))
  (Rendering|Material|SetMaterial (Variables|/Game/Project/Core/InteractOBJ/BP_CoreOBJ.BP_CoreOBJ_C|GetStaticMesh _ref_insertedglass) 3 _previewmat))

(fn PresetZoominGroup
  (Utilities|Array|Add (Variables|Default|GetWidgetTriggerGroup) (Variables|Default|GetZoomTrigger_Main)))

(fn SwitchMeshCollisionProfile
  (params (bIsBlock :type Boolean))
  (if bIsBlock
    (LocalVariables|SetL_ProfileName "StandByMode")
    (else
      (LocalVariables|SetL_ProfileName "NoCollision")))
  (Collision|SetCollisionProfileName (Variables|/Game/Project/BluePrints/InteractOBJ/BP_OBJ_TA.BP_OBJ_TA_C|GetKey_TriggerArea (Variables|Default|GetREF_OBJ%20TA)) (LocalVariables|GetL_ProfileName) true :!class /Script/Engine.PrimitiveComponent))