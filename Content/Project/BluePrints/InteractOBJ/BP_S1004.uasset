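; BP_S1004 is the Stage 1 goal door, with a glowing diamond and a stage-clear trigger.
; Film events play sounds and timelines that swing both door leaves open or ramp the diamond's dynamic material, which starts dark from construction.
; When the player enters StageCompleteTA, it destroys the trigger, locks control through REFStageManager, reverses a depth-of-field timeline on the character's post-process, then calls Stage1ClearEvent.
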(event OnComponentBeginOverlap(StageCompleteTA)
  (params (OverlappedComponent :type Primitive%20Component%20Object%20Reference) (OtherActor :type Actor%20Object%20Reference) (OtherComp :type Primitive%20Component%20Object%20Reference) (OtherBodyIndex :type Integer) (bFromSweep :type Boolean) (SweepResult :type Hit%20Result%20Structure%20%28by%20ref%29))
  (bind _returnvalue (Game|GetPlayerCharacter 0))
  (if (== OtherActor _returnvalue)
    (Components|DestroyComponent OverlappedComponent)
    (Default|PlayerCtrlLockbyStageClearTA (Variables|Default|GetREF_StageManager))
    (bind _asbp_first_person_character (Utilities|Casting|CastToBP_FirstPersonCharacter _returnvalue))
    (bind (_direction _sensorwidth _focaldistance) (Timeline|Timeline ReverseFromEnd)
      (:Update
        (Utilities|Struct|SetmembersinPostProcessSettings (Variables|/Script/Engine.PostProcessComponent|GetSettings (Variables|/Game/ProjectDefault/FirstPerson/Blueprints/BP_FirstPersonCharacter.BP_FirstPersonCharacter_C|GetPostProcessComponent _asbp_first_person_character)) _sensorwidth _focaldistance))
      (:Finished
        (Default|Stage1ClearEvent (Variables|Default|GetREF_StageManager))))))

(event Custom|Film_GoalDoorOpen
  (bind _sm_door_l (Variables|Default|GetSM_Door_L))
  (bind _sm_door_r (Variables|Default|GetSM_Door_R))
  (bind _relativerotation (Variables|/Script/Engine.SceneComponent|GetRelativeRotation _sm_door_l))
  (bind _relativerotation_2 (Variables|/Script/Engine.SceneComponent|GetRelativeRotation _sm_door_r))
  (Audio|SpawnSoundAttached "/Game/Project/Audio/MetaSoundSource/SE/MSS_FinalDoor.MSS_FinalDoor" (Variables|Default|GetSM_Door_Frame) "None" "0, 0, 0" "0, 0, 0" "KeepRelativeOffset" false 1.0 1.0 0.0 0 0)
  (bind _axis (Timeline|DoorAxis PlayFromStart)
    (:Update
      (Transformation|SetRelativeRotation _sm_door_l (Math|Rotator|MakeRotator (.roll _relativerotation) (.pitch _relativerotation) (* (Math|Float|Lerp 0.0 9e+01 _axis) -1.0)) false false)
      (Transformation|SetRelativeRotation _sm_door_r (Math|Rotator|MakeRotator (.roll _relativerotation_2) (.pitch _relativerotation_2) (Math|Float|Lerp 0.0 9e+01 _axis)) false false))
    (:Finished
      (Audio|SpawnSoundAttached "/Game/Project/Audio/MetaSoundSource/SE/MSS_FinalDoorFinish.MSS_FinalDoorFinish" (Variables|Default|GetSM_Door_Frame) "None" "0, 0, 0" "0, 0, 0" "KeepRelativeOffset" false 1.0 1.0 0.0 0 0))))

(event Custom|Film_GoalDiamondGlow
  (bind _diamond_doortop (Variables|Default|GetDiamond_DoorTop))
  (Audio|SpawnSoundAttached "/Game/Project/Audio/MetaSoundSource/SE/MSS_DiamondActivate.MSS_DiamondActivate" (Variables|Default|GetSM_Door_Frame) "None" "0, 0, 0" "0, 0, 0" "KeepRelativeOffset" false 1.0 1.0 0.0 0 0)
  (bind (_direction _enable _speed) (Timeline|DiamondState PlayFromStart)
    (:Update
      (Rendering|Material|SetScalarParameterValue _diamond_doortop "Enable" _enable :!class /Script/Engine.MaterialInstanceDynamic)
      (Rendering|Material|SetScalarParameterValue _diamond_doortop "Speed" _speed :!class /Script/Engine.MaterialInstanceDynamic))))

(event EventBeginPlay)

(event Collision|EventActorBeginOverlap
  (params (OtherActor :type Actor%20Object%20Reference)))

(fn ConstructionScript
  (bind _returnvalue (Rendering|Material|CreateDynamicMaterialInstance "/Game/Project/Artist/Scene/Material/Door_Diamond.Door_Diamond" "None" "None" :!class /Script/Engine.KismetMaterialLibrary))
  (bind _output_get (Variables|Default|SetDiamond_DoorTop _returnvalue))
  (Rendering|Material|SetScalarParameterValue _output_get "Enable" 0.0 :!class /Script/Engine.MaterialInstanceDynamic)
  (Rendering|Material|SetScalarParameterValue _output_get "Speed" 0.0 :!class /Script/Engine.MaterialInstanceDynamic)
  (Rendering|Material|SetMaterial (Variables|Default|GetSM_Door_Frame) 5 (Variables|Default|GetDiamond_DoorTop)))