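; Interactable certify machine puzzle with a draggable push handle, glass code check and final item reward.
; Vertical mouse drag drives the push-key animation speed, whose socket height moves the handle and scrubs spring and bellow geometry caches through start-time offsets.
; Check functions match inserted glass totem values against codes, block pushing on mismatch, or reveal the item and play the activation sequence.
; Timelines animate the film's lights and planet glow.
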(event OnClicked(SM_Pusher_Handle)
  (params (TouchedComponent :type Primitive%20Component%20Object%20Reference) (ButtonPressed :type Key%20Structure))
  ;[1 1 1] Mesh Control Event
  (Variables|Default|SetbIsDragSlider true)
  (Variables|/Game/ProjectDefault/FirstPerson/Blueprints/BP_FirstPersonCharacter.BP_FirstPersonCharacter_C|SetCurrentInteract (Variables|Default|GetPlayer) self))

(event Custom|Play%20Film%20Setup
  (bind _ref_fog (Variables|Default|GetREF_Fog))
  (bind _component (Variables|/Script/Engine.ExponentialHeightFog|GetComponent _ref_fog))
  (Utilities|FlowControl|Sequence
    (:then_0
      (Default|OpenFilmHint (Variables|/Game/ProjectDefault/FirstPerson/Blueprints/BP_FirstPersonCharacter.BP_FirstPersonCharacter_C|GetREF_CoreHUD (Variables|Default|GetPlayer)) false)
      (Default|ToggleInputFilm (Variables|Default|GetPlayer) true false)
      (Default|CallFilmStart))
    (:then_1
      (Utilities|FlowControl|Delay 1.0)
      (Class|ExponentialHeightFogComponent|SetVolumetricFog _component true)
      (Class|ExponentialHeightFogComponent|SetFogDensity _component 1.0)
      (bind _outactor (Sequencer|Player|CreateLevelSequencePlayer "/Game/Project/Film/LS_CertifyMachine_Activate.LS_CertifyMachine_Activate" (Utilities|Struct|MakeMovieSceneSequencePlaybackSettings false "(Value=0)" 1.0 0.0 false false true true false false false false)))
      (bind _output_get (Variables|Default|SetCurrentSequence (Variables|/Script/LevelSequence.LevelSequenceActor|GetSequencePlayer _outactor)))
      (bind _output_get_2 (Variables|/Game/ProjectDefault/FirstPerson/Blueprints/BP_FirstPersonCharacter.BP_FirstPersonCharacter_C|SetCurrentSequence (Variables|Default|GetPlayer) _output_get))
      (Sequencer|Player|Play _output_get_2 :!class /Script/MovieScene.MovieSceneSequencePlayer)
      (Variables|Default|SetbPlayingFilm true))))

(event Custom|Film_PlanetMatValueCtrl
  ;[1 1 1] Film Effect
  (bind _glowmat (Timeline|Timeline Play)
    (:Update
      (Rendering|Material|SetScalarParameterValue (Variables|Default|GetREF_CertifyPlanetMat) "Emit Value" _glowmat :!class /Script/Engine.MaterialInstanceDynamic))))

(event Custom|Film_PointlightPlaying
  ;[1 1 1] Film Effect
  (bind (_direction _intensity _radius) (Timeline|Pointlight_Intensity PlayFromStart)
    (:Update
      (Rendering|Components|Light|SetIntensity (Variables|Default|GetPointLight) (Math|Float|Lerp 0.0 5e+02 _intensity))
      (Class|PointLightComponent|SetSourceRadius (Variables|Default|GetPointLight) (Math|Float|Lerp 0.0 1.5e+02 _radius)))))

(event Custom|Film_SpotlightPlaying
  ;[1 1 1] Film Effect
  (bind _intense (Timeline|Spotlight_Intensity PlayFromStart)
    (:Update
      (Rendering|Components|Light|SetIntensity (Variables|Default|GetSpotLight) _intense))
    (:Finished
      (bind _focus (Timeline|Spotlight_ConeAngle PlayFromStart)
        (:Update
          (Rendering|Lighting|SetOuterConeAngle (Variables|Default|GetSpotLight) _focus))))))

(event EventBeginPlay
  (|CallParentFunction)
  (CallFunction|PresetAnim))

(event EventInteractEnd
  (Variables|/Game/ProjectDefault/FirstPerson/Blueprints/BP_FirstPersonCharacter.BP_FirstPersonCharacter_C|SetCurrentInteract (Variables|Default|GetPlayer) self)
  (switch int (Variables|Default|GetZoomInPart)
    (:0
      (Variables|Default|SetbIsDragSlider false))))

(event EventZoomin
  (params (ZoomComponent :type Actor%20Component%20Object%20Reference))
  (|CallParentFunction ZoomComponent))

(event EventZoomOut
  (|CallParentFunction))

(event EventTick
  (params (DeltaSeconds :type Float%20%28single-precision%29))
  (CallFunction|FilmStateCheck)
  (if (not (Variables|Default|GetbIsStandByState))
    (switch int (Variables|Default|GetZoomInPart)
      (:0
        (CallFunction|PushCheckState)))))

(fn ConstructionScript
  (|CallParentFunction)
  (CallFunction|PresetValue)
  (CallFunction|PresetGeo))

(fn CheckCreateFinalItemRequest
  (if (Variables|Default|GetbBlockRequest)
    (Variables|Default|SetbBlockRequest false)
    (elif (== (Variables|Default|GetLatestDir_Push) 0)
      (Variables|Default|SetbBlockRequest true)
      (bind _output_get (Variables|/Game/Project/Artist/Machine/Mesh/SK_Certify_Push_Key_Skeleton_AnimBlueprint.SK_Certify_Push_Key_Skeleton_AnimBlueprint_C|SetSpeedRating (Variables|Default|GetREF_PushKeyAnimGraph) 0.0))
      (Variables|Default|SetLatestRating _output_get)
      (Variables|Default|SetbBlockByWrongCode false)
      (else
        (Utilities|FlowControl|Sequence
          (:then_0
            (Variables|Default|SetbFinalItemIsCreate true)
            (Rendering|SetActorHiddenInGame (Variables|Default|GetFinalItem) false)
            (Audio|SpawnSoundAttached "/Game/Project/Audio/MetaSoundSource/SE/MSS_MetalLock_1.MSS_MetalLock_1" (Variables|Default|GetSK_Certify_Push_Key) "None" "0, 0, 0" "0, 0, 0" "KeepRelativeOffset" false 1.0 1.0 0.0 0 0))
          (:then_1
            (CallFunction|PlayFilmSetup)))))))

(fn CheckNeedBlockbyCode
  (if (not (Variables|Default|GetbGlassCodeIsMatch))
    (Variables|Default|SetbBlockByWrongCode true)
    (bind _output_get (Variables|/Game/Project/Artist/Machine/Mesh/SK_Certify_Push_Key_Skeleton_AnimBlueprint.SK_Certify_Push_Key_Skeleton_AnimBlueprint_C|SetSpeedRating (Variables|Default|GetREF_PushKeyAnimGraph) 0.0))
    (Variables|Default|SetLatestRating _output_get)
    (if (== (Variables|Default|GetLatestDir_Push) 1)
      (Audio|SpawnSoundAttached "/Game/Project/Audio/MetaSoundSource/SE/MSS_MetalLock_6.MSS_MetalLock_6" (Variables|Default|GetSK_Certify_Push_Key) "None" "0, 0, 0" "0, 0, 0" "KeepRelativeOffset" false 1.0 1.0 0.0 0 0))))

(fn CertifySingleTotemValue
  (params (GlassValue :type ST%20Glass%20Value%20Structure))
  (LocalVariables|SetL_CurrentValue GlassValue)
  (Utilities|FlowControl|Sequence
    (:then_0
      (LocalVariables|SetL_CurrentSpline (.SplineTotem (Utilities|Struct|BreakST_GlassValue (LocalVariables|GetL_CurrentValue))))
      (LocalVariables|SetL_CurrentRotate (.Code_Rotate (Utilities|Struct|BreakST_GlassValue (LocalVariables|GetL_CurrentValue))))
      (LocalVariables|SetL_CurrentExpand (.Code_Expand (Utilities|Struct|BreakST_GlassValue (LocalVariables|GetL_CurrentValue))))
      (LocalVariables|SetL_CurrentDistance (.Code_Distance (Utilities|Struct|BreakST_GlassValue (LocalVariables|GetL_CurrentValue))))
      (LocalVariables|SetL_CurrentScale (.Code_Scale (Utilities|Struct|BreakST_GlassValue (LocalVariables|GetL_CurrentValue)))))
    (:then_1
      (bind (_array_element _array_index) (Utilities|Array|ForEachLoopwithBreak (Variables|Default|GetGlassMatchCode_QuickTest) :!label _label)
        (:LoopBody
          (bind _output_get (LocalVariables|SetL_REF_ST_GlassMatchCode _array_element))
          (LocalVariables|SetL_Index _array_index)
          (if (and (not (.bAlreadyMatch (Utilities|Struct|BreakST_GlassMatchCode _output_get))) (== (.Match_Spline (Utilities|Struct|BreakST_GlassMatchCode _output_get)) (LocalVariables|GetL_CurrentSpline)))
            (bind _bismatch (CallFunction|CertifyIntDataIsInclude (LocalVariables|GetL_CurrentRotate) (.Match_Rotate (Utilities|Struct|BreakST_GlassMatchCode (LocalVariables|GetL_REF_ST_GlassMatchCode)))))
            (bind _bismatch_2 (CallFunction|CertifyIntDataIsInclude (LocalVariables|GetL_CurrentExpand) (.Match_Expand (Utilities|Struct|BreakST_GlassMatchCode (LocalVariables|GetL_REF_ST_GlassMatchCode)))))
            (bind _bismatch_3 (CallFunction|CertifyIntDataIsInclude (LocalVariables|GetL_CurrentDistance) (.Match_Distance (Utilities|Struct|BreakST_GlassMatchCode (LocalVariables|GetL_REF_ST_GlassMatchCode)))))
            (bind _bismatch_4 (CallFunction|CertifyIntDataIsInclude (LocalVariables|GetL_CurrentScale) (.Match_Scale (Utilities|Struct|BreakST_GlassMatchCode (LocalVariables|GetL_REF_ST_GlassMatchCode)))))
            (if (Math|Boolean|ANDBoolean _bismatch_4 _bismatch_3 _bismatch_2 _bismatch)
              (bind _structout (Utilities|Struct|SetmembersinST_GlassMatchCode (LocalVariables|GetL_REF_ST_GlassMatchCode) true))
              (Utilities|Array|SetArrayElem (Variables|Default|GetGlassMatchCode_QuickTest) (LocalVariables|GetL_Index) _structout)
              (goto _label Break))))))))

(fn CertifyWholeMatchCode
  (Variables|Default|SetbGlassCodeIsMatch true)
  (bind _array_element (Utilities|Array|ForEachLoopwithBreak (Variables|Default|GetGlassMatchCode_QuickTest) :!label _label)
    (:LoopBody
      (if (not (Utilities|Struct|BreakST_GlassMatchCode _array_element))
        (Variables|Default|SetbGlassCodeIsMatch false)
        (goto _label Break)))))

(fn CertifyIntDataIsInclude
  (params (CurrentValue :type Integer) (MatchCodes :type Array%20of%20Integers))
  (bind _array_element (Utilities|Array|ForEachLoopwithBreak MatchCodes :!label _label)
    (:LoopBody
      (if (== _array_element CurrentValue)
        (LocalVariables|SetL_IsMatch true)
        (goto _label Break)))
    (:Completed
      (return (LocalVariables|GetL_IsMatch)))))

(fn CertifyStartCheckMatchCode
  (for _array_element (Utilities|Struct|BreakST_GlassData (Variables|Default|GetInsertedGlass))
    (CallFunction|CertifySingleTotemValue _array_element))
  (CallFunction|CertifyWholeMatchCode))

(fn FilmStateCheck
  (bind _ref_fog (Variables|Default|GetREF_Fog))
  (bind _currentsequence (Variables|Default|GetCurrentSequence))
  (bind _component (Variables|/Script/Engine.ExponentialHeightFog|GetComponent _ref_fog))
  (if (Variables|Default|GetbPlayingFilm)
    (Utilities|IsValid _currentsequence
      (:Is%20Valid
        (bind _output_get (Variables|Default|SetbPlayingFilm (Audio|Components|Audio|IsPlaying _currentsequence)))
        (if (not _output_get)
          (Default|CallFilmEnd)
          (Class|ExponentialHeightFogComponent|SetVolumetricFog _component false)
          (Class|ExponentialHeightFogComponent|SetFogDensity _component 0.0))))))

(fn GeoCachePlayer
  (params (Percentage :type Float%20%28double-precision%29))
  (bind _output_get (LocalVariables|SetL_Percentage Percentage))
  (if (>= _output_get 0.998)
    (LocalVariables|SetL_Percentage 0.999))
  (Utilities|FlowControl|Sequence
    (:then_0
      (Class|GeometryCacheComponent|SetStartTimeOffset (Variables|Default|GetCertify_Spring) (* (Variables|Default|GetGeoDuration-Spring) (LocalVariables|GetL_Percentage))))
    (:then_1
      (Class|GeometryCacheComponent|SetStartTimeOffset (Variables|Default|GetCertify_Bellow) (* (Variables|Default|GetGeoDuration-Bellow) (LocalVariables|GetL_Percentage))))
    (:then_2
      (if (Math|Float|NearlyEqual(Float) (LocalVariables|GetL_Percentage) (Math|Conversions|ToFloat(Integer) (Variables|Default|GetLatestDir_Push)) 1e-06)
        (Audio|SpawnSoundAttached "/Game/Project/Audio/MetaSoundSource/SE/MSS_MetalLock_10.MSS_MetalLock_10" (Variables|Default|GetSK_Certify_Push_Key) "None" "0, 0, 0" "0, 0, 0" "KeepRelativeOffset" false 1.0 1.0 0.0 0 0)))))

(fn PresetAnim
  (Utilities|FlowControl|Sequence
    (:then_0
      (bind _assk_certify_push_key_skeleton_anim_blueprint (Utilities|Casting|CastToSK_Certify_Push_Key_Skeleton_AnimBlueprint (Components|SkeletalMesh|GetAnimInstance (Variables|Default|GetSK_Certify_Push_Key))))
      (Variables|Default|SetREF_PushKeyAnimGraph _assk_certify_push_key_skeleton_anim_blueprint))
    (:then_1
      (bind _assk_certify_sun_planet_skeleton_anim_blueprint (Utilities|Casting|CastToSK_Certify_Sun_Planet_Skeleton_AnimBlueprint (Components|SkeletalMesh|GetAnimInstance (Variables|Default|GetSK_Certify_Sun_Planet))))
      (Variables|Default|SetREF_PlanetAnimGraph _assk_certify_sun_planet_skeleton_anim_blueprint))
    (:then_2
      (bind _returnvalue (Rendering|Material|CreateDynamicMaterialInstance (Variables|Default|GetSK_Certify_Sun_Planet) 4 "/Game/Project/Artist/Machine/Material/Certify_Planet_00.Certify_Planet_00" "None" :!class /Script/Engine.PrimitiveComponent))
      (Variables|Default|SetREF_CertifyPlanetMat _returnvalue))))

(fn PresetGeo
  (Utilities|FlowControl|Sequence
    (:then_0
      (Variables|Default|SetGeoDuration-Spring (Variables|/Script/GeometryCache.GeometryCacheComponent|GetDuration (Variables|Default|GetCertify_Spring))))
    (:then_1
      (Variables|Default|SetGeoDuration-Bellow (Variables|/Script/GeometryCache.GeometryCacheComponent|GetDuration (Variables|Default|GetCertify_Bellow))))))

(fn PresetValue
  (Utilities|FlowControl|Sequence
    (:then_0
      (bind _asbp_core_ta_glass (Utilities|Casting|CastToBP_CoreTA_Glass (Variables|/Script/Engine.ChildActorComponent|GetChildActor (Variables|Default|GetFinalNotch))))
      (bind _output_get (Variables|Default|SetREF_FinalNotch _asbp_core_ta_glass))
      (Default|PlaceOffsetLocation _output_get "-27.691159,-6.745552,5.462831" "0.000000,-90.000000,0.000000"))
    (:then_1
      (Utilities|Array|Add (Variables|Default|GetWidgetTriggerGroup) (Variables|Default|GetWidget%20Trigger_FinalHandle))
      (Utilities|Array|Add (Variables|Default|GetWidgetTriggerGroup) (Variables|Default|GetWidget%20Trigger_FinalItem)))
    (:then_2
      (bind _asbp_core_item (Utilities|Casting|CastToBP_CoreITEM (Variables|/Script/Engine.ChildActorComponent|GetChildActor (Variables|Default|GetFinalItemMesh))))
      (bind _output_get_2 (Variables|Default|SetFinalItem _asbp_core_item))
      (Collision|SetCollisionProfileName (Variables|/Game/Project/Core/InteractOBJ/BP_CoreOBJ.BP_CoreOBJ_C|GetStaticMesh _output_get_2) "NoCollision" true :!class /Script/Engine.PrimitiveComponent)
      (Rendering|SetActorHiddenInGame (Variables|Default|GetFinalItem) true))))

(fn PushCheckState
  (if (and (Variables|Default|GetbIsDragSlider) (not (Variables|Default|GetbFinalItemIsCreate)))
    (if (Variables|Default|GetbHasUpdateMousePivot)
      (CallFunction|PushDragViaInput)
      (else
        (Variables|Default|SetbHasUpdateMousePivot true)
        (CallFunction|UpdateTriggerMousePivot)))
    (else
      (Variables|Default|SetbHasUpdateMousePivot false)
      (Variables|Default|SetLatestDir_Push 0)
      (if (> (Variables|Default|GetGeoPercentage) 0.0)
        (CallFunction|PushFinishRemainOffset (Variables|Default|GetbFinalItemIsCreate))))))

(fn PushDragViaInput
  (bind _returnvalue (Game|GetPlayerController 0))
  (bind _triggermousepivot (Variables|S9009|GetTriggerMousePivot))
  (bind _ref_pushkeyanimgraph (Variables|Default|GetREF_PushKeyAnimGraph))
  (bind _sm_pusher_handle (Variables|Default|GetSM_Pusher_Handle))
  (bind _returnvalue_2 (Transformation|GetWorldLocation _sm_pusher_handle))
  (bind _worldlocation (Game|Player|ConvertMouseLocationToWorldSpace _returnvalue))
  (bind _screenlocation (Class|PlayerController|ProjectWorldLocationtoScreen _returnvalue _worldlocation false))
  (if (!= (.y _screenlocation) (.y _triggermousepivot))
    (LocalVariables|SetL_IsFowardDir (> (.y _screenlocation) (.y _triggermousepivot)))
    (if (not (Variables|Default|GetbBlockByWrongCode))
      (Utilities|FlowControl|Sequence
        (:then_0
          (if (LocalVariables|GetL_IsFowardDir)
            (LocalVariables|SetL_SpeedDir 1.0)
            (LocalVariables|SetL_CurrentDir 1)
            (else
              (LocalVariables|SetL_SpeedDir -1.0)
              (LocalVariables|SetL_CurrentDir -1)))
          (Variables|Default|SetLatestDir_Push (LocalVariables|GetL_CurrentDir)))
        (:then_1
          (bind _output_get (Variables|/Game/Project/Artist/Machine/Mesh/SK_Certify_Push_Key_Skeleton_AnimBlueprint.SK_Certify_Push_Key_Skeleton_AnimBlueprint_C|SetSpeedRating _ref_pushkeyanimgraph (+ (* (Utilities|Time|GetWorldDeltaSeconds) (LocalVariables|GetL_SpeedDir)) (Variables|/Game/Project/Artist/Machine/Mesh/SK_Certify_Push_Key_Skeleton_AnimBlueprint.SK_Certify_Push_Key_Skeleton_AnimBlueprint_C|GetSpeedRating _ref_pushkeyanimgraph))))
          (bind _output_get_2 (Variables|Default|SetLatestRating _output_get))
          (if (>= _output_get_2 1.0)
            (bind _output_get_3 (Variables|/Game/Project/Artist/Machine/Mesh/SK_Certify_Push_Key_Skeleton_AnimBlueprint.SK_Certify_Push_Key_Skeleton_AnimBlueprint_C|SetSpeedRating (Variables|Default|GetREF_PushKeyAnimGraph) 1.0))
            (Variables|Default|SetLatestRating _output_get_3)
            (elif (<= _output_get_2 -1.0)
              (bind _output_get_4 (Variables|/Game/Project/Artist/Machine/Mesh/SK_Certify_Push_Key_Skeleton_AnimBlueprint.SK_Certify_Push_Key_Skeleton_AnimBlueprint_C|SetSpeedRating (Variables|Default|GetREF_PushKeyAnimGraph) -1.0))
              (Variables|Default|SetLatestRating _output_get_4))))
        (:then_2
          (LocalVariables|SetL_PushOffset (- 72.705 (.z (Transformation|GetSocketLocation (Variables|Default|GetSK_Certify_Push_Key) "Push"))))
          (Transformation|SetWorldLocation _sm_pusher_handle (Math|Vector|MakeVector (.x _returnvalue_2) (.y _returnvalue_2) (- 1.6e+02 (LocalVariables|GetL_PushOffset))) false false)
          (bind _output_get_5 (Variables|Default|SetGeoPercentage (Math|Float|Clamp(Float) (/ (LocalVariables|GetL_PushOffset) (Variables|Default|GetPushPos_Range)))))
          (CallFunction|GeoCachePlayer _output_get_5))))))

(fn PushFinishRemainOffset
  (params (bGoingOpen :type Boolean))
  (bind _ref_pushkeyanimgraph (Variables|Default|GetREF_PushKeyAnimGraph))
  (bind _sm_pusher_handle (Variables|Default|GetSM_Pusher_Handle))
  (bind _returnvalue (Transformation|GetWorldLocation _sm_pusher_handle))
  (bind _output_get (LocalVariables|SetL_GoingOpen bGoingOpen))
  (if _output_get
    (LocalVariables|SetL_SpeedDir 1.0)
    (else
      (LocalVariables|SetL_SpeedDir -1.0)
      (if (> (Variables|Default|GetLatestRating) 0.0)
        (bind _output_get_2 (Variables|/Game/Project/Artist/Machine/Mesh/SK_Certify_Push_Key_Skeleton_AnimBlueprint.SK_Certify_Push_Key_Skeleton_AnimBlueprint_C|SetSpeedRating (Variables|Default|GetREF_PushKeyAnimGraph) 0.0))
        (Variables|Default|SetLatestRating _output_get_2))))
  (bind _output_get_3 (Variables|/Game/Project/Artist/Machine/Mesh/SK_Certify_Push_Key_Skeleton_AnimBlueprint.SK_Certify_Push_Key_Skeleton_AnimBlueprint_C|SetSpeedRating _ref_pushkeyanimgraph (+ (* (Utilities|Time|GetWorldDeltaSeconds) (LocalVariables|GetL_SpeedDir)) (Variables|/Game/Project/Artist/Machine/Mesh/SK_Certify_Push_Key_Skeleton_AnimBlueprint.SK_Certify_Push_Key_Skeleton_AnimBlueprint_C|GetSpeedRating _ref_pushkeyanimgraph))))
  (bind _output_get_4 (Variables|Default|SetLatestRating _output_get_3))
  (if (>= _output_get_4 1.0)
    (bind _output_get_5 (Variables|/Game/Project/Artist/Machine/Mesh/SK_Certify_Push_Key_Skeleton_AnimBlueprint.SK_Certify_Push_Key_Skeleton_AnimBlueprint_C|SetSpeedRating (Variables|Default|GetREF_PushKeyAnimGraph) 1.0))
    (Variables|Default|SetLatestRating _output_get_5)
    (elif (<= _output_get_4 -1.0)
      (bind _output_get_6 (Variables|/Game/Project/Artist/Machine/Mesh/SK_Certify_Push_Key_Skeleton_AnimBlueprint.SK_Certify_Push_Key_Skeleton_AnimBlueprint_C|SetSpeedRating (Variables|Default|GetREF_PushKeyAnimGraph) -1.0))
      (Variables|Default|SetLatestRating _output_get_6)))
  (LocalVariables|SetL_PushOffset (- 72.705 (.z (Transformation|GetSocketLocation (Variables|Default|GetSK_Certify_Push_Key) "Push"))))
  (Transformation|SetWorldLocation _sm_pusher_handle (Math|Vector|MakeVector (.x _returnvalue) (.y _returnvalue) (- 1.6e+02 (LocalVariables|GetL_PushOffset))) false false)
  (bind _output_get_7 (Variables|Default|SetGeoPercentage (Math|Float|Clamp(Float) (/ (LocalVariables|GetL_PushOffset) (Variables|Default|GetPushPos_Range)))))
  (CallFunction|GeoCachePlayer _output_get_7))

(fn UpdateTriggerMousePivot
  (bind _returnvalue (Game|GetPlayerController 0))
  (Variables|S9009|SetTriggerMousePivot (.ScreenLocation (Class|PlayerController|ProjectWorldLocationtoScreen _returnvalue (.WorldLocation (Game|Player|ConvertMouseLocationToWorldSpace _returnvalue)) false))))

(fn AssignZoomPos
  (params (ZoomInComp :type Object%20Object%20Reference))
  (bind (_array_element _array_index) (Utilities|Array|ForEachLoopwithBreak (Variables|Default|GetWidgetTriggerGroup) :!label _label)
    (:LoopBody
      (if (== _array_element ZoomInComp)
        (Variables|Default|SetZoomInPart _array_index)
        (goto _label Break)))
    (:Completed
      (Transformation|SetRelativeTransform (Variables|Default|GetZoomInCamera) (Utilities|Array|Get(acopy) (Variables|Default|GetZoomInPoint) (Variables|Default|GetZoomInPart)) false false)
      (CallFunction|SwitchMeshCollisionProfile true))))

(fn SwitchMeshCollisionProfile
  (params (bIsBlock :type Boolean))
  (bind _ref_finalnotch (Variables|Default|GetREF_FinalNotch))
  (bind _ref_insertedglass (Variables|/Game/Project/Core/GameSystem/BP_CoreTA_Glass.BP_CoreTA_Glass_C|GetREF_InsertedGLASS _ref_finalnotch))
  (bind _output_get (LocalVariables|SetIsBlock bIsBlock))
  (if _output_get
    (LocalVariables|SetL_ProfileName "StandByMode")
    (else
      (LocalVariables|SetL_ProfileName "NoCollision")))
  (switch int (Variables|Default|GetZoomInPart)
    (:0
      (Collision|SetCollisionProfileName (Variables|Default|GetSM_Pusher_Handle) (LocalVariables|GetL_ProfileName) true :!class /Script/Engine.PrimitiveComponent)
      (Utilities|IsValid _ref_insertedglass
        (:Is%20Valid
          (Collision|SetCollisionProfileName (Variables|/Game/Project/Core/InteractOBJ/BP_CoreOBJ.BP_CoreOBJ_C|GetStaticMesh _ref_insertedglass) (LocalVariables|GetL_ProfileName) true :!class /Script/Engine.PrimitiveComponent))))
    (:1
      (if (and (Variables|Default|GetbFinalItemIsCreate) (LocalVariables|GetIsBlock))
        (Collision|SetCollisionProfileName (Variables|/Game/Project/Core/InteractOBJ/BP_CoreOBJ.BP_CoreOBJ_C|GetStaticMesh (Variables|Default|GetFinalItem)) "StandByMode" true :!class /Script/Engine.PrimitiveComponent)
        (else
          (Collision|SetCollisionProfileName (Variables|/Game/Project/Core/InteractOBJ/BP_CoreOBJ.BP_CoreOBJ_C|GetStaticMesh (Variables|Default|GetFinalItem)) "NoCollision" true :!class /Script/Engine.PrimitiveComponent))))))