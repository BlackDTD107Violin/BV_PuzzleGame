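; BP_S9006 is an interactable mixer scale slider, linked to its parent BP_S9002 panel, that sets the units of an inserted GLASS.
; While GLASS is inserted, dragging the mouse diagonally slides the handle between limits with sounds, tracking the nearest unit.
; On release it eases onto that unit and updates the panel's code; received codes and resets also set it.
; Tick rotates the scale modules to show the selected count.
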(event OnClicked(SM_Mixer_Scale_Handle)
  (params (TouchedComponent :type Primitive%20Component%20Object%20Reference) (ButtonPressed :type Key%20Structure))
  (Variables|Default|SetbIsDragging true)
  (Variables|/Game/ProjectDefault/FirstPerson/Blueprints/BP_FirstPersonCharacter.BP_FirstPersonCharacter_C|SetCurrentInteract (Variables|Default|GetPlayer) self))

(event EventBeginPlay
  (|CallParentFunction)
  (CallFunction|PresetScaleModuleGroup))

(event EventTick
  (params (DeltaSeconds :type Float%20%28single-precision%29))
  (CallFunction|CheckState)
  (CallFunction|CheckScaleModule))

(event EventInteractEnd
  (Variables|Default|SetbIsDragging false))

(fn ConstructionScript
  (|CallParentFunction)
  (bind _asbp_s9002 (Utilities|Casting|CastToBP_S9002 (Actor|GetParentActor)))
  (Variables|Default|SetREF_%20InteractPanel _asbp_s9002))

(fn BacktoDefault
  (Variables|Default|SetInsertedGLASSUnits 0)
  (Variables|Default|SetbHasInsertedGLASS false)
  (Default|UpdateGLASSCodefromEachFunc (Variables|Default|GetREF_%20InteractPanel))
  (Variables|Default|SetTargetUnitsPosX (Utilities|Array|Get(acopy) (Variables|Default|GetUnits) (Variables|Default|GetInsertedGLASSUnits)))
  (Variables|Default|SetbGetTargetUnit true))

(fn CheckNearestUnits
  (LocalVariables|SetL_CurrentPosX (.x (Variables|/Script/Engine.SceneComponent|GetRelativeLocation (Variables|Default|GetSM_Mixer_Scale_Handle))))
  (for (_array_element _array_index) (Variables|Default|GetUnits)
    (bind _output_get (LocalVariables|SetL_CurDis (Math|Float|Absolute(Float) (- _array_element (LocalVariables|GetL_CurrentPosX)))))
    (if (<= _output_get (LocalVariables|GetL_MinDis))
      (Variables|Default|SetTargetUnitsPosX _array_element)
      (Variables|Default|SetInsertedGLASSUnits _array_index)
      (LocalVariables|SetL_MinDis (LocalVariables|GetL_CurDis)))))

(fn CheckScaleModule
  (for (_array_element _array_index) (Variables|Default|GetScaleModuleGroup)
    (LocalVariables|SetL_CurrentModule _array_element)
    (if (> (Variables|Default|GetInsertedGLASSUnits) _array_index)
      (LocalVariables|SetL_TargetAngle 45.0)
      (else
        (LocalVariables|SetL_TargetAngle 0.0)))
    (Utilities|FlowControl|Sequence
      (:then_0
        (Transformation|SetRelativeRotation (LocalVariables|GetL_CurrentModule) (Math|Interpolation|RInterpTo (Variables|/Script/Engine.SceneComponent|GetRelativeRotation (LocalVariables|GetL_CurrentModule)) (Math|Rotator|MakeRotator (.roll (Variables|/Script/Engine.SceneComponent|GetRelativeRotation (LocalVariables|GetL_CurrentModule))) (.pitch (Variables|/Script/Engine.SceneComponent|GetRelativeRotation (LocalVariables|GetL_CurrentModule))) (LocalVariables|GetL_TargetAngle)) (Utilities|Time|GetWorldDeltaSeconds) 8.0) false false))
      (:then_1
        (if (and (== (LocalVariables|GetL_TargetAngle) 45.0) (<= (- (LocalVariables|GetL_TargetAngle) (.yaw (Variables|/Script/Engine.SceneComponent|GetRelativeRotation (LocalVariables|GetL_CurrentModule)))) 0.1))
          (Transformation|SetRelativeRotation (LocalVariables|GetL_CurrentModule) (Math|Rotator|MakeRotator (.roll (Variables|/Script/Engine.SceneComponent|GetRelativeRotation (LocalVariables|GetL_CurrentModule))) (.pitch (Variables|/Script/Engine.SceneComponent|GetRelativeRotation (LocalVariables|GetL_CurrentModule))) (LocalVariables|GetL_TargetAngle)) false false :!label _label)
          (elif (and (== (LocalVariables|GetL_TargetAngle) 0.0) (<= (- (.yaw (Variables|/Script/Engine.SceneComponent|GetRelativeRotation (LocalVariables|GetL_CurrentModule))) (LocalVariables|GetL_TargetAngle)) 0.1))
            (goto _label)))))))

(fn CheckState
  (if (Variables|Default|GetbHasInsertedGLASS)
    (if (Variables|Default|GetbIsDragging)
      (if (Variables|Default|GetbHasUpdateMousePivot)
        (CallFunction|DragViaInput)
        (CallFunction|CheckNearestUnits)
        (else
          (Variables|Default|SetbHasUpdateMousePivot true)
          (CallFunction|UpdateTriggerMousePivot)))
      (else
        (if (Variables|Default|GetbGetTargetUnit) :!label _label
          _
          (else
            (CallFunction|CheckNearestUnits)
            (Variables|Default|SetbGetTargetUnit true)
            (Default|UpdateGLASSCodefromEachFunc (Variables|Default|GetREF_%20InteractPanel))))
        (CallFunction|GotoTargetUnit)))
    (else
      (goto _label))))

(fn DragViaInput
  (bind _returnvalue (Game|GetPlayerController 0))
  (bind _sm_mixer_scale_handle (Variables|Default|GetSM_Mixer_Scale_Handle))
  (bind _triggermousepivot (Variables|Default|GetTriggerMousePivot))
  (bind _worldlocation (Game|Player|ConvertMouseLocationToWorldSpace _returnvalue))
  (bind _screenlocation (Class|PlayerController|ProjectWorldLocationtoScreen _returnvalue _worldlocation false))
  (bind _returnvalue_2 (- _screenlocation _triggermousepivot))
  (bind (_x _y) (Math|Vector2D|BreakVector2D _returnvalue_2))
  (bind (_x_2 _y_2) (Math|Vector2D|BreakVector2D _returnvalue_2))
  (if (and (> _x 0.0) (> _y 0.0))
    (Variables|Default|SetbGetTargetUnit false)
    (LocalVariables|SetL_LimitedLocation 15.5)
    (if (not (Class|KismetMathLibrary|LinearColorIsNearEqual (Math|Conversions|ToLinearColor(Float) (.x (Variables|/Script/Engine.SceneComponent|GetRelativeLocation (Variables|Default|GetSM_Mixer_Scale_Handle)))) (Math|Conversions|ToLinearColor(Float) (LocalVariables|GetL_LimitedLocation)) 0.0001))
      (Transformation|AddLocalOffset (Variables|Default|GetSM_Mixer_Scale_Handle) (Math|Vector|MakeVector (Variables|Default|GetDefaultSpeed) 0.0 0.0) false false)
      (if (>= (.x (Variables|/Script/Engine.SceneComponent|GetRelativeLocation (Variables|Default|GetSM_Mixer_Scale_Handle))) (LocalVariables|GetL_LimitedLocation))
        (Transformation|SetRelativeLocation _sm_mixer_scale_handle (Math|Vector|MakeVector (LocalVariables|GetL_LimitedLocation) (* (LocalVariables|GetL_LimitedLocation) -1.0) (.z (Variables|/Script/Engine.SceneComponent|GetRelativeLocation _sm_mixer_scale_handle))) false false :!label _label)
        (Variables|Default|SetbHasUpdateMousePivot false)
        (if (not (Variables|Default|GetbMeshReachLimit))
          (Variables|Default|SetbMeshReachLimit true)
          (Audio|SpawnSoundAttached "/Game/Project/Audio/MetaSoundSource/SE/MSS_MetalLock_4.MSS_MetalLock_4" (Variables|Default|GetSM_Mixer_Scale_Handle) "None" "0, 0, 0" "0, 0, 0" "KeepRelativeOffset" false 1.0 1.0 0.0 0 0)
          (Variables|Default|SetbSoundPlaying false)
          (CallFunction|StopContinuedSE (Variables|Default|GetAudioEnable_Handle)))
        (else
          (CallFunction|UpdateTriggerMousePivot :!label _label_2)
          (Variables|Default|SetbMeshReachLimit false)
          (if (not (Variables|Default|GetbSoundPlaying))
            (Variables|Default|SetbSoundPlaying true)
            (bind _returnvalue_3 (Audio|SpawnSoundAttached "/Game/Project/Audio/MetaSoundSource/SE/MSS_ScaleSlider_7.MSS_ScaleSlider_7" (Variables|Default|GetSM_Mixer_Scale_Handle) "None" "0, 0, 0" "0, 0, 0" "KeepRelativeOffset" false 1.0 1.0 0.0 0 0))
            (Variables|Default|SetAudioEnable_Handle _returnvalue_3)))))
    (elif (and (< _x_2 0.0) (< _y_2 0.0))
      (Variables|Default|SetbGetTargetUnit false)
      (LocalVariables|SetL_LimitedLocation 1.65)
      (if (not (Class|KismetMathLibrary|LinearColorIsNearEqual (Math|Conversions|ToLinearColor(Float) (.x (Variables|/Script/Engine.SceneComponent|GetRelativeLocation (Variables|Default|GetSM_Mixer_Scale_Handle)))) (Math|Conversions|ToLinearColor(Float) (LocalVariables|GetL_LimitedLocation)) 0.0001))
        (Transformation|AddLocalOffset (Variables|Default|GetSM_Mixer_Scale_Handle) (Math|Vector|MakeVector (* (Variables|Default|GetDefaultSpeed) -1.0) 0.0 0.0) false false)
        (if (<= (.x (Variables|/Script/Engine.SceneComponent|GetRelativeLocation (Variables|Default|GetSM_Mixer_Scale_Handle))) (LocalVariables|GetL_LimitedLocation))
          (goto _label)
          (else
            (goto _label_2)))))))

(fn GotoTargetUnit
  (bind _targetunitsposx (Variables|Default|GetTargetUnitsPosX))
  (bind _sm_mixer_scale_handle (Variables|Default|GetSM_Mixer_Scale_Handle))
  (bind _targetunitsposx_2 (Variables|Default|GetTargetUnitsPosX))
  (bind _sm_mixer_scale_handle_2 (Variables|Default|GetSM_Mixer_Scale_Handle))
  (Utilities|FlowControl|Sequence
    (:then_0
      (Transformation|SetRelativeLocation (Variables|Default|GetSM_Mixer_Scale_Handle) (Math|Interpolation|VInterpTo (Variables|/Script/Engine.SceneComponent|GetRelativeLocation _sm_mixer_scale_handle_2) (Math|Vector|MakeVector _targetunitsposx (* _targetunitsposx -1.0) (.z (Variables|/Script/Engine.SceneComponent|GetRelativeLocation _sm_mixer_scale_handle_2))) (Utilities|Time|GetWorldDeltaSeconds) 4.0) false false))
    (:then_1
      (if (<= (Math|Float|Absolute(Float) (- (.x (Variables|/Script/Engine.SceneComponent|GetRelativeLocation (Variables|Default|GetSM_Mixer_Scale_Handle))) (Variables|Default|GetTargetUnitsPosX))) 0.2)
        (Transformation|SetRelativeLocation _sm_mixer_scale_handle (Math|Vector|MakeVector _targetunitsposx_2 (* _targetunitsposx_2 -1.0) (.z (Variables|/Script/Engine.SceneComponent|GetRelativeLocation _sm_mixer_scale_handle))) false false)
        (Variables|Default|SetbHasUpdateMousePivot false)
        (if (not (Variables|Default|GetbMeshReachLimit))
          (Variables|Default|SetbMeshReachLimit true)
          (Audio|SpawnSoundAttached "/Game/Project/Audio/MetaSoundSource/SE/MSS_MetalLock_4.MSS_MetalLock_4" (Variables|Default|GetSM_Mixer_Scale_Handle) "None" "0, 0, 0" "0, 0, 0" "KeepRelativeOffset" false 1.0 1.0 0.0 0 0)
          (Variables|Default|SetbSoundPlaying false)
          (CallFunction|StopContinuedSE (Variables|Default|GetAudioEnable_Handle)))))))

(fn PresetScaleModuleGroup
  (Utilities|FlowControl|Sequence
    (:then_0
      (Utilities|Array|Add (Variables|Default|GetScaleModuleGroup) (Variables|Default|GetSM_Mixer_Scale_Module01))
      (Utilities|Array|Add (Variables|Default|GetScaleModuleGroup) (Variables|Default|GetSM_Mixer_Scale_Module02))
      (Utilities|Array|Add (Variables|Default|GetScaleModuleGroup) (Variables|Default|GetSM_Mixer_Scale_Module03)))
    (:then_1
      (Utilities|Array|Add (Variables|Default|GetScaleModuleGroup) (Variables|Default|GetSM_Mixer_Scale_Module04))
      (Utilities|Array|Add (Variables|Default|GetScaleModuleGroup) (Variables|Default|GetSM_Mixer_Scale_Module05))
      (Utilities|Array|Add (Variables|Default|GetScaleModuleGroup) (Variables|Default|GetSM_Mixer_Scale_Module06)))))

(fn PresetValue)

(fn ReceiveGLASScode
  (params (Code :type Integer))
  (bind _output_get (Variables|Default|SetInsertedGLASSUnits Code))
  (Variables|Default|SetTargetUnitsPosX (Utilities|Array|Get(acopy) (Variables|Default|GetUnits) _output_get))
  (Variables|Default|SetbGetTargetUnit true)
  (Variables|Default|SetbHasInsertedGLASS true)
  (Default|UpdateGLASSCodefromEachFunc (Variables|Default|GetREF_%20InteractPanel)))

(fn UpdateTriggerMousePivot
  (bind _returnvalue (Game|GetPlayerController 0))
  (Variables|Default|SetTriggerMousePivot (.ScreenLocation (Class|PlayerController|ProjectWorldLocationtoScreen _returnvalue (.WorldLocation (Game|Player|ConvertMouseLocationToWorldSpace _returnvalue)) false))))