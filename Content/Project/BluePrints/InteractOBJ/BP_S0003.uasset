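; Tutorial lockbox interactable that the player zooms into and opens by dragging first the lock, then the cover, to reach a key item.
; Zoom events blend the view, toggle movement input and collision, and drive tutorial prompts.
; Tick compares screen-space mouse Y to rotate each pivot, easing it to its end angle when released past a threshold.
; The cover blocks the child-actor key and updates its CanTake state while dragged.
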(event OnClicked(Cover)
  (params (TouchedComponent :type Primitive%20Component%20Object%20Reference) (ButtonPressed :type Key%20Structure))
  (if (and (not (Variables|Default|GetbCoverIsFinish)) (Variables|Default|GetbLockIsFinish))
    (Variables|Default|SetbIsDraggingCover true)
    (Variables|/Game/ProjectDefault/FirstPerson/Blueprints/BP_FirstPersonCharacterTutorial.BP_FirstPersonCharacterTutorial_C|SetCurrentInteract (Variables|Default|GetPlayer_Tutorial) self)))

(event OnClicked(Lock)
  (params (TouchedComponent :type Primitive%20Component%20Object%20Reference) (ButtonPressed :type Key%20Structure))
  (if (not (Variables|Default|GetbLockIsFinish))
    (Variables|Default|SetbIsDraggingLock true)
    (Variables|/Game/ProjectDefault/FirstPerson/Blueprints/BP_FirstPersonCharacterTutorial.BP_FirstPersonCharacterTutorial_C|SetCurrentInteract (Variables|Default|GetPlayer_Tutorial) self)))

(event EventBeginPlay
  (bind _returnvalue (Game|GetPlayerController 0))
  (|CallParentFunction)
  (bind _asbp_first_person_character_tutorial (Utilities|Casting|CastToBP_FirstPersonCharacterTutorial (Game|GetPlayerCharacter 0)))
  (Variables|Default|SetPlayer_Tutorial _asbp_first_person_character_tutorial)
  (Input|EnableInput _returnvalue)
  (Variables|/Script/Engine.PlayerController|SetbEnableClickEvents _returnvalue true)
  (Variables|/Script/Engine.PlayerController|SetbEnableMouseOverEvents _returnvalue true)
  (CallFunction|AssignZoominGroup)
  (Variables|/Game/ProjectDefault/FirstPerson/Blueprints/BP_FirstPersonCharacterTutorial.BP_FirstPersonCharacterTutorial_C|SetUnlockBox (Variables|Default|GetPlayer_Tutorial) self))

(event EventInteractEnd
  (CallFunction|CancelingDrag)
  (Variables|/Game/ProjectDefault/FirstPerson/Blueprints/BP_FirstPersonCharacterTutorial.BP_FirstPersonCharacterTutorial_C|SetCurrentInteract (Variables|Default|GetPlayer_Tutorial) self)
  (Variables|Default|SetbSoundPlaying false))

(event EventZoomin
  (params (ZoomComponent :type Actor%20Component%20Object%20Reference))
  (bind _returnvalue (Game|GetPlayerController 0))
  (bind _player_tutorial (Variables|Default|GetPlayer_Tutorial))
  (Game|Player|SetViewTargetwithBlend (Game|GetPlayerController 0) self 0.5 "VTBlend_Linear" 0.0 true)
  (Input|SetIgnoreMoveInput _returnvalue true)
  (Input|SetIgnoreLookInput _returnvalue true)
  (Default|ClearGamePromptUIView (Variables|Default|GetPlayer_Tutorial))
  (Collision|SetCollisionProfileName (Variables|Default|GetZoom%20Trigger_Main) "NoCollision" true :!class /Script/Engine.PrimitiveComponent)
  (for _array_element (Variables|Default|GetMeshGroup)
    (Collision|SetCollisionProfileName _array_element "StandByMode" true :!class /Script/Engine.PrimitiveComponent)
    (if (not (Variables|Default|GetbItemTutorHasTrigger))
      (Variables|Default|SetbItemTutorHasTrigger true)
      (Utilities|FlowControl|Delay 0.5)
      (Default|ArriveTutorialTA _player_tutorial)
      (Default|ClearGamePromptUIView _player_tutorial))))

(event EventZoomOut
  (bind _returnvalue (Game|GetPlayerController 0))
  (bind _player_tutorial (Variables|Default|GetPlayer_Tutorial))
  (Game|Player|SetViewTargetwithBlend (Game|GetPlayerController 0) (Game|GetPlayerCharacter 0) 0.5 "VTBlend_Linear" 0.0 true)
  (if (== (Variables|/Game/ProjectDefault/FirstPerson/Blueprints/BP_FirstPersonCharacterTutorial.BP_FirstPersonCharacterTutorial_C|GetCurrentGoal _player_tutorial) 8)
    (Default|CloseTutor (Variables|/Game/ProjectDefault/FirstPerson/Blueprints/BP_FirstPersonCharacterTutorial.BP_FirstPersonCharacterTutorial_C|GetREF_CoreHUDTutorial _player_tutorial)))
  (Input|ResetIgnoreMoveInput _returnvalue)
  (Input|ResetIgnoreLookInput _returnvalue)
  (Utilities|FlowControl|Delay 0.5)
  (Collision|SetCollisionProfileName (Variables|Default|GetZoom%20Trigger_Main) "StandByMode" true :!class /Script/Engine.PrimitiveComponent)
  (for _array_element (Variables|Default|GetMeshGroup)
    (Collision|SetCollisionProfileName _array_element "NoCollision" true :!class /Script/Engine.PrimitiveComponent)))

(event EventTick
  (params (DeltaSeconds :type Float%20%28single-precision%29))
  (if (Variables|Default|GetbLockIsFinish)
    (if (not (Variables|Default|GetbCoverIsFinish))
      (CallFunction|CheckCoverState))
    (else
      (CallFunction|CheckLockState))))

(fn ConstructionScript
  (|CallParentFunction)
  (CallFunction|PresetItemMesh))

(fn AssignZoominGroup
  (Utilities|Array|Add (Variables|Default|GetMeshGroup) (Variables|Default|GetCover))
  (Utilities|Array|Add (Variables|Default|GetMeshGroup) (Variables|Default|GetLock)))

(fn CancelingDrag
  (Variables|Default|SetbIsDraggingLock false)
  (Variables|Default|SetbIsDraggingCover false)
  (Variables|Default|SetbHasUpdateMousePivot false))

(fn CheckCoverState
  (if (Variables|Default|GetbIsDraggingCover)
    (if (Variables|Default|GetbHasUpdateMousePivot)
      (CallFunction|DragCoverViaInput)
      (CallFunction|CheckCanTakeItem (Variables|Default|GetCover) false (.roll (Variables|/Script/Engine.SceneComponent|GetRelativeRotation (Variables|Default|GetCoverPivot))) -45.0)
      (else
        (Variables|Default|SetbHasUpdateMousePivot true)
        (CallFunction|UpdateTriggerMousePivot)))
    (elif (<= (.roll (Variables|/Script/Engine.SceneComponent|GetRelativeRotation (Variables|Default|GetCoverPivot))) -6e+01)
      (CallFunction|FinishRemainingAngleCover))))

(fn CheckLockState
  (if (Variables|Default|GetbIsDraggingLock)
    (if (Variables|Default|GetbHasUpdateMousePivot)
      (CallFunction|DragLockViaInput)
      (else
        (Variables|Default|SetbHasUpdateMousePivot true)
        (CallFunction|UpdateTriggerMousePivot)))
    (elif (<= (.roll (Variables|/Script/Engine.SceneComponent|GetRelativeRotation (Variables|Default|GetLockPivot))) -9e+01)
      (CallFunction|FinishRemainingAngleLock))))

(fn DragCoverViaInput
  (bind _returnvalue (Game|GetPlayerController 0))
  (bind _triggermousepivot (Variables|Default|GetTriggerMousePivot))
  (bind _worldlocation (Game|Player|ConvertMouseLocationToWorldSpace _returnvalue))
  (bind _screenlocation (Class|PlayerController|ProjectWorldLocationtoScreen _returnvalue _worldlocation false))
  (if (not (Variables|Default|GetbCoverIsFinish))
    (if (!= (.y _screenlocation) (.y _triggermousepivot))
      (if (> (.y _screenlocation) (.y _triggermousepivot))
        (Transformation|AddLocalRotation (Variables|Default|GetCoverPivot) (Math|Rotator|MakeRotator (Variables|Default|GetRotateSpeed) 0.0 0.0) false false)
        (if (>= (.roll (Variables|/Script/Engine.SceneComponent|GetRelativeRotation (Variables|Default|GetCoverPivot))) 0.0)
          (Transformation|SetRelativeRotation (Variables|Default|GetCoverPivot) "0, 0, 0" false false)
          (else
            (CallFunction|UpdateTriggerMousePivot)
            (if (not (Variables|Default|GetbSoundPlaying))
              (Variables|Default|SetbSoundPlaying true)
              (Audio|SpawnSoundAttached "/Game/Project/Audio/MetaSoundSource/SE/MSS_S0003_CoverSlide.MSS_S0003_CoverSlide" (Variables|Default|GetCoverPivot) "None" "0, 0, 0" "0, 0, 0" "KeepRelativeOffset" false 1.0 1.0 0.0 0 0))))
        (else
          (Transformation|AddLocalRotation (Variables|Default|GetCoverPivot) (Math|Rotator|MakeRotator (* (Variables|Default|GetRotateSpeed) -1.0) 0.0 0.0) false false)
          (if (<= (Class|KismetMathLibrary|ClampAxis (.roll (Variables|/Script/Engine.SceneComponent|GetRelativeRotation (Variables|Default|GetCoverPivot)))) 2.7e+02)
            (Variables|Default|SetbCoverIsFinish true)
            (CallFunction|CancelingDrag)
            (Collision|SetCollisionProfileName (Variables|Default|GetStaticMesh) "TRICKignore" true :!class /Script/Engine.PrimitiveComponent)
            (Audio|SpawnSoundAttached "/Game/Project/Audio/MetaSoundSource/SE/MSS_S0003_CoverFinish.MSS_S0003_CoverFinish" (Variables|Default|GetCoverPivot) "None" "0, 0, 0" "0, 0, 0" "KeepRelativeOffset" false 1.0 1.0 0.0 0 0)
            (Variables|Default|SetbSoundPlaying false)
            (else
              (CallFunction|UpdateTriggerMousePivot)
              (if (not (Variables|Default|GetbSoundPlaying))
                (Variables|Default|SetbSoundPlaying true)
                (Audio|SpawnSoundAttached "/Game/Project/Audio/MetaSoundSource/SE/MSS_S0003_CoverSlide.MSS_S0003_CoverSlide" (Variables|Default|GetCoverPivot) "None" "0, 0, 0" "0, 0, 0" "KeepRelativeOffset" false 1.0 1.0 0.0 0 0)))))))))

(fn DragLockViaInput
  (bind _returnvalue (Game|GetPlayerController 0))
  (bind _triggermousepivot (Variables|Default|GetTriggerMousePivot))
  (bind _worldlocation (Game|Player|ConvertMouseLocationToWorldSpace _returnvalue))
  (bind _screenlocation (Class|PlayerController|ProjectWorldLocationtoScreen _returnvalue _worldlocation false))
  (if (not (Variables|Default|GetbLockIsFinish))
    (if (!= (.y _screenlocation) (.y _triggermousepivot))
      (if (> (.y _screenlocation) (.y _triggermousepivot))
        (Transformation|AddLocalRotation (Variables|Default|GetLockPivot) (Math|Rotator|MakeRotator (Variables|Default|GetRotateSpeed) 0.0 0.0) false false)
        (if (>= (.roll (Variables|/Script/Engine.SceneComponent|GetRelativeRotation (Variables|Default|GetLockPivot))) 0.0)
          (Transformation|SetRelativeRotation (Variables|Default|GetLockPivot) "0, 0, 0" false false)
          (else
            (CallFunction|UpdateTriggerMousePivot)
            (if (not (Variables|Default|GetbSoundPlaying))
              (Variables|Default|SetbSoundPlaying true)
              (Audio|SpawnSoundAttached "/Game/Project/Audio/MetaSoundSource/SE/MSS_S0003_LockSlide.MSS_S0003_LockSlide" (Variables|Default|GetLockPivot) "None" "0, 0, 0" "0, 0, 0" "KeepRelativeOffset" false 1.0 1.0 0.0 0 0))))
        (else
          (Transformation|AddLocalRotation (Variables|Default|GetLockPivot) (Math|Rotator|MakeRotator (* (Variables|Default|GetRotateSpeed) -1.0) 0.0 0.0) false false)
          (if (<= (Class|KismetMathLibrary|ClampAxis (.roll (Variables|/Script/Engine.SceneComponent|GetRelativeRotation (Variables|Default|GetLockPivot)))) 1.8e+02)
            (Variables|Default|SetbLockIsFinish true)
            (CallFunction|CancelingDrag)
            (Audio|SpawnSoundAttached "/Game/Project/Audio/MetaSoundSource/SE/MSS_S0003_LockFinish.MSS_S0003_LockFinish" (Variables|Default|GetLockPivot) "None" "0, 0, 0" "0, 0, 0" "KeepRelativeOffset" false 1.0 1.0 0.0 0 0)
            (Variables|Default|SetbSoundPlaying false)
            (else
              (CallFunction|UpdateTriggerMousePivot)
              (if (not (Variables|Default|GetbSoundPlaying))
                (Variables|Default|SetbSoundPlaying true)
                (Audio|SpawnSoundAttached "/Game/Project/Audio/MetaSoundSource/SE/MSS_S0003_LockSlide.MSS_S0003_LockSlide" (Variables|Default|GetLockPivot) "None" "0, 0, 0" "0, 0, 0" "KeepRelativeOffset" false 1.0 1.0 0.0 0 0)))))))))

(fn FinishRemainingAngleCover
  (bind _coverpivot (Variables|Default|GetCoverPivot))
  (bind _coverpivot_2 (Variables|Default|GetCoverPivot))
  (bind _relativerotation (Variables|/Script/Engine.SceneComponent|GetRelativeRotation _coverpivot_2))
  (bind _relativerotation_2 (Variables|/Script/Engine.SceneComponent|GetRelativeRotation _coverpivot))
  (Utilities|FlowControl|Sequence
    (:then_0
      (Transformation|SetRelativeRotation (Variables|Default|GetCoverPivot) (Math|Interpolation|RInterpTo (Variables|/Script/Engine.SceneComponent|GetRelativeRotation (Variables|Default|GetCoverPivot)) (Math|Rotator|MakeRotator -9e+01 (.pitch _relativerotation) (.yaw _relativerotation)) (Utilities|Time|GetWorldDeltaSeconds) 4.0) false false))
    (:then_1
      (if (<= (.roll (Variables|/Script/Engine.SceneComponent|GetRelativeRotation (Variables|Default|GetCoverPivot))) -89.0)
        (Transformation|SetRelativeRotation (Variables|Default|GetCoverPivot) (Math|Rotator|MakeRotator -9e+01 (.pitch _relativerotation_2) (.yaw _relativerotation_2)) false false)
        (Variables|Default|SetbCoverIsFinish true)
        (CallFunction|CancelingDrag)
        (Collision|SetCollisionProfileName (Variables|Default|GetStaticMesh) "TRICKignore" true :!class /Script/Engine.PrimitiveComponent)
        (Audio|SpawnSoundAttached "/Game/Project/Audio/MetaSoundSource/SE/MSS_S0003_CoverFinish.MSS_S0003_CoverFinish" (Variables|Default|GetCoverPivot) "None" "0, 0, 0" "0, 0, 0" "KeepRelativeOffset" false 1.0 1.0 0.0 0 0)
        (Variables|Default|SetbSoundPlaying false)))))

(fn FinishRemainingAngleLock
  (bind _lockpivot (Variables|Default|GetLockPivot))
  (bind _lockpivot_2 (Variables|Default|GetLockPivot))
  (bind _relativerotation (Variables|/Script/Engine.SceneComponent|GetRelativeRotation _lockpivot))
  (bind _relativerotation_2 (Variables|/Script/Engine.SceneComponent|GetRelativeRotation _lockpivot_2))
  (Utilities|FlowControl|Sequence
    (:then_0
      (Transformation|SetRelativeRotation (Variables|Default|GetLockPivot) (Math|Interpolation|RInterpTo (Variables|/Script/Engine.SceneComponent|GetRelativeRotation (Variables|Default|GetLockPivot)) (Math|Rotator|MakeRotator -1.8e+02 (.pitch _relativerotation) (.yaw _relativerotation)) (Utilities|Time|GetWorldDeltaSeconds) 4.0) false false))
    (:then_1
      (if (<= (.roll (Variables|/Script/Engine.SceneComponent|GetRelativeRotation (Variables|Default|GetLockPivot))) -179.0)
        (Transformation|SetRelativeRotation (Variables|Default|GetLockPivot) (Math|Rotator|MakeRotator -1.8e+02 (.pitch _relativerotation_2) (.yaw _relativerotation_2)) false false)
        (Variables|Default|SetbLockIsFinish true)
        (CallFunction|CancelingDrag)
        (Audio|SpawnSoundAttached "/Game/Project/Audio/MetaSoundSource/SE/MSS_S0003_LockFinish.MSS_S0003_LockFinish" (Variables|Default|GetLockPivot) "None" "0, 0, 0" "0, 0, 0" "KeepRelativeOffset" false 1.0 1.0 0.0 0 0)
        (Variables|Default|SetbSoundPlaying false)))))

(fn UpdateTriggerMousePivot
  (bind _returnvalue (Game|GetPlayerController 0))
  (Variables|Default|SetTriggerMousePivot (.ScreenLocation (Class|PlayerController|ProjectWorldLocationtoScreen _returnvalue (.WorldLocation (Game|Player|ConvertMouseLocationToWorldSpace _returnvalue)) false))))

(fn PresetItemMesh
  (bind _asbp_core_item (Utilities|Casting|CastToBP_CoreITEM (Variables|/Script/Engine.ChildActorComponent|GetChildActor (Variables|Default|GetKey))))
  (bind _output_get (Variables|Default|SetREF_K0001 _asbp_core_item))
  (Utilities|Array|Add (Variables|/Game/Project/Core/InteractOBJ/BP_CoreITEM.BP_CoreITEM_C|GetBlockBy _output_get) (Variables|Default|GetCover)))

(fn CheckCanTakeItem
  (params (CurrentMesh :type Static%20Mesh%20Component%20Object%20Reference) (bOpenDirIsPositive :type Boolean) (CurrentValue :type Float%20%28double-precision%29) (BorderValue :type Float%20%28double-precision%29))
  (if bOpenDirIsPositive
    (Variables|/Game/Project/Core/InteractOBJ/BP_CoreITEM.BP_CoreITEM_C|SetbCanTake (Variables|Default|GetREF_K0001) (>= CurrentValue BorderValue))
    (else
      (Variables|/Game/Project/Core/InteractOBJ/BP_CoreITEM.BP_CoreITEM_C|SetbCanTake (Variables|Default|GetREF_K0001) (<= CurrentValue BorderValue)))))