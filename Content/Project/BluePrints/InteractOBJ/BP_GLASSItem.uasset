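; Inspectable glass item that plugs into the mixer, calculate, extract and certify slots of the game's machines.
; Entering inspection detaches it from its current slot, resetting input or output side state and signalling that the glass is consumed.
; Exiting inspection switches off the scene capture matching its inserted side via the glass manager.
; Three dynamic diamond materials, created at BeginPlay, light up and animate according to the glass's inherit layer.
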(event EventBeginPlay
  (|CallParentFunction)
  (CallFunction|CreateDiamondMat))

(event EventEnterInspector
  (|CallParentFunction)
  (bind _currentinsertedta (Variables|Default|GetCurrentInsertedTA)
    (:then
      (bind _side (Default|PickOutGLASS _currentinsertedta))
      (Default|ResetPlaceOffset (Variables|Default|GetCurrentInsertedTA))
      (if (or (Utilities|Enum|Equal(Enum) _side "NewEnumerator3") (Utilities|Enum|Equal(Enum) _side "NewEnumerator5"))
        (CallFunction|RemovefromOutputSide)
        (else
          (CallFunction|RemovefromInputSide))))
    (:else)))

(event EventExitInspector
  (|CallParentFunction)
  (CallFunction|StopMatchSceneCapture (Variables|Default|GetGlassInsertedState))
  (Variables|Default|SetGlassInsertedState "NewEnumerator0"))

(fn ConstructionScript
  (|CallParentFunction))

(fn RemovefromInputSide
  (switch Utilities|FlowControl|Switch|SwitchonE_GlassSideState (Variables|/Game/Project/Core/GameSystem/BP_CoreTA_Glass.BP_CoreTA_Glass_C|GetGlassTAside (Variables|Default|GetCurrentInsertedTA))
    (:NewEnumerator1
      (Default|RemoveGlassTAside (Variables|Default|GetCurrentInsertedTA) (Variables|/Game/Project/Core/GameSystem/BP_CoreTA_Glass.BP_CoreTA_Glass_C|GetGlassTAside (Variables|Default|GetCurrentInsertedTA)) :!label _label))
    (:NewEnumerator2
      (goto _label))
    (:NewEnumerator4
      (Default|UpdateGLASSCode (Variables|Default|GetCurrentInsertedTA))
      (Default|RemoveGlassTAside (Variables|Default|GetCurrentInsertedTA) (Variables|/Game/Project/Core/GameSystem/BP_CoreTA_Glass.BP_CoreTA_Glass_C|GetGlassTAside (Variables|Default|GetCurrentInsertedTA))))
    (:NewEnumerator6
      (Variables|/Game/Project/BluePrints/InteractOBJ/BP_S9009.BP_S9009_C|SetbGlassCodeIsMatch (Variables|/Game/Project/Core/GameSystem/BP_CoreTA_Glass.BP_CoreTA_Glass_C|GetREF_CertifyMachine (Variables|Default|GetCurrentInsertedTA)) false)))
  (Variables|/Game/Project/Core/GameSystem/BP_CoreTA_Glass.BP_CoreTA_Glass_C|SetREF_InsertedGLASS (Variables|Default|GetCurrentInsertedTA) 0)
  (Variables|Default|SetCurrentInsertedTA 0)
  (Default|CallConsumeThisGlass self))

(fn RemovefromOutputSide
  (bind _ref_mainmachine (Variables|/Game/Project/Core/GameSystem/BP_CoreTA_Glass.BP_CoreTA_Glass_C|GetREF_MainMachine (Variables|Default|GetCurrentInsertedTA))
    (:then
      (Variables|/Game/Project/BluePrints/InteractOBJ/BP_S9001.BP_S9001_C|SetbMixNotchIsEmpty _ref_mainmachine true))
    (:else
      _))
  (Variables|/Game/Project/Core/GameSystem/BP_CoreTA_Glass.BP_CoreTA_Glass_C|SetREF_InsertedGLASS (Variables|Default|GetCurrentInsertedTA) 0)
  (Variables|Default|SetCurrentInsertedTA 0)
  (Default|CallConsumeThisGlass self))

(fn CreateDiamondMat
  (Utilities|FlowControl|Sequence
    (:then_0
      (bind _returnvalue (Rendering|Material|CreateDynamicMaterialInstance "/Game/Project/Artist/KeyObj/Material/Slider_Diamond00.Slider_Diamond00" "None" "None" :!class /Script/Engine.KismetMaterialLibrary))
      (Utilities|Array|Add (Variables|Default|GetDiamondGroups) _returnvalue))
    (:then_1
      (bind _returnvalue_2 (Rendering|Material|CreateDynamicMaterialInstance "/Game/Project/Artist/KeyObj/Material/Slider_Diamond02.Slider_Diamond02" "None" "None" :!class /Script/Engine.KismetMaterialLibrary))
      (Utilities|Array|Add (Variables|Default|GetDiamondGroups) _returnvalue_2))
    (:then_2
      (bind _returnvalue_3 (Rendering|Material|CreateDynamicMaterialInstance "/Game/Project/Artist/KeyObj/Material/Slider_Diamond01.Slider_Diamond01" "None" "None" :!class /Script/Engine.KismetMaterialLibrary))
      (Utilities|Array|Add (Variables|Default|GetDiamondGroups) _returnvalue_3))
    (:then_3
      (for _array_element (Variables|Default|GetDiamondGroups)
        (Rendering|Material|SetScalarParameterValue _array_element "Enable" 0.0 :!class /Script/Engine.MaterialInstanceDynamic)
        (Rendering|Material|SetScalarParameterValue _array_element "Speed" 0.0 :!class /Script/Engine.MaterialInstanceDynamic)))))

(fn SetInheritDiamond
  (LocalVariables|SetL_Layer (.inheritlayer (Variables|Default|GetThisGlass)))
  (for _index (range 0 2)
    (bind _output_get (LocalVariables|SetL_LoopIndex _index))
    (if (< _output_get (LocalVariables|GetL_Layer))
      (Rendering|Material|SetScalarParameterValue (Utilities|Array|Get(acopy) (Variables|Default|GetDiamondGroups) (LocalVariables|GetL_LoopIndex)) "Enable" 1.0 :!class /Script/Engine.MaterialInstanceDynamic)
      (Rendering|Material|SetScalarParameterValue (Utilities|Array|Get(acopy) (Variables|Default|GetDiamondGroups) (LocalVariables|GetL_LoopIndex)) "Speed" 0.1 :!class /Script/Engine.MaterialInstanceDynamic)
      (else
        (Rendering|Material|SetScalarParameterValue (Utilities|Array|Get(acopy) (Variables|Default|GetDiamondGroups) (LocalVariables|GetL_LoopIndex)) "Enable" 0.0 :!class /Script/Engine.MaterialInstanceDynamic)
        (Rendering|Material|SetScalarParameterValue (Utilities|Array|Get(acopy) (Variables|Default|GetDiamondGroups) (LocalVariables|GetL_LoopIndex)) "Speed" 0.0 :!class /Script/Engine.MaterialInstanceDynamic)))
    (Rendering|Material|SetMaterial (Variables|Default|GetStaticMesh) (+ (LocalVariables|GetL_LoopIndex) 4) (Utilities|Array|Get(acopy) (Variables|Default|GetDiamondGroups) (LocalVariables|GetL_LoopIndex)))))

(fn StopMatchSceneCapture
  (params (Side :type E_GlassSideState%20Enum :default "NewEnumerator0"))
  (switch Utilities|FlowControl|Switch|SwitchonE_GlassSideState Side
    (:NewEnumerator1
      (LocalVariables|SetL_SideIndex 2))
    (:NewEnumerator2
      (LocalVariables|SetL_SideIndex 3))
    (:NewEnumerator3
      (LocalVariables|SetL_SideIndex 4))
    (:NewEnumerator4
      (LocalVariables|SetL_SideIndex 1))
    (:NewEnumerator5
      (LocalVariables|SetL_SideIndex 0))
    (:NewEnumerator6
      (LocalVariables|SetL_SideIndex 6)))
  (Default|SwitchStateSceneCaptureScene (Variables|Default|GetREF_GlassManager) false (LocalVariables|GetL_SideIndex)))