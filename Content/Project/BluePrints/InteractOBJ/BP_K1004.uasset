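; BP_K1004 is an interactable object with a simulated sloshing liquid, driven through a dynamic material created at construction.
; Each Tick, UpdateLiquidSurface springs a clamped position behind the actor for height and lateral slosh, and springs a dummy component's rotation toward up for surface tilt.
; The blended height and direction feed the material's LiquidHeight and LiquidDirection parameters.
; Inspector and extraction-glow events only call the parent.
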(event EventBeginPlay
  (|CallParentFunction))

(event EventItemExtractGlowing
  (params (bIsExtracting :type Boolean))
  (|CallParentFunction bIsExtracting))

(event EventEnterInspector
  (|CallParentFunction))

(event EventExitInspector
  (|CallParentFunction))

(event EventTick
  (params (DeltaSeconds :type Float%20%28single-precision%29))
  (bind _ref_fluidmat (Variables|Default|GetREF_FluidMat))
  (bind (_liquidheight _liquiddirction) (CallFunction|UpdateLiquidSurface))
  (Rendering|Material|SetScalarParameterValue _ref_fluidmat "LiquidHeight" _liquidheight :!class /Script/Engine.MaterialInstanceDynamic)
  (Rendering|Material|SetVectorParameterValue _ref_fluidmat "LiquidDirection" (Math|Conversions|ToLinearColor(Vector) _liquiddirction) :!class /Script/Engine.MaterialInstanceDynamic))

(fn ConstructionScript
  (|CallParentFunction)
  (bind _returnvalue (Rendering|Material|CreateDynamicMaterialInstance (Variables|Default|GetFluidMatTest) "None" "None" :!class /Script/Engine.KismetMaterialLibrary))
  (bind _output_get (Variables|Default|SetREF_FluidMat _returnvalue))
  (Rendering|Material|SetMaterial (Variables|Default|GetStaticMesh) 0 _output_get))

(fn UpdateLiquidSurface
  (bind _liquidlocationoffset (Variables|Default|GetLiquidLocationOffset))
  (LocalVariables|SetL_CurrentLocation (Transformation|GetActorLocation))
  (Utilities|FlowControl|Sequence
    (:then_0
      (bind _returnvalue (Class|KismetMathLibrary|VectorSpringInterp (Variables|Default|GetSpringLiquidLocation) (LocalVariables|GetL_CurrentLocation) (Variables|Default|GetSpringStateLiquidLocation) 1.5e+02 0.2 (Utilities|Time|GetWorldDeltaSeconds) 1.0 0.1 true (- (LocalVariables|GetL_CurrentLocation) _liquidlocationoffset) (+ (LocalVariables|GetL_CurrentLocation) _liquidlocationoffset) true))
      (bind _output_get (Variables|Default|SetSpringLiquidLocation _returnvalue))
      (LocalVariables|SetL_FinalLiquidHeight (- (.z _output_get) (.Z (Math|Vector|BreakVector (LocalVariables|GetL_CurrentLocation))))))
    (:then_1
      (bind _returnvalue_2 (Class|KismetMathLibrary|QuaternionSpringInterp (Math|Conversions|ToQuaternion(Rotator) (Transformation|GetWorldRotation (Variables|Default|GetDummySurfaceDirection))) (Math|Conversions|ToQuaternion(Rotator) (Math|Vector|VectorUp)) (Variables|Default|GetSpringStateLiquidRotation) 1.5e+02 0.2 (Utilities|Time|GetWorldDeltaSeconds) 1.0 0.1 true))
      (Transformation|SetWorldRotation (Variables|Default|GetDummySurfaceDirection) (Class|KismetMathLibrary|QuatRotator _returnvalue_2) false false)
      (return (LocalVariables|GetL_FinalLiquidHeight) (Math|Vector|Lerp(Vector) (Math|Vector|Lerp(Vector) (Math|Rotator|GetRotationXVector (Class|KismetMathLibrary|QuatRotator _returnvalue_2)) (Math|Vector|MakeVector (.x (- (Variables|Default|GetSpringLiquidLocation) (LocalVariables|GetL_CurrentLocation))) (.y (- (Variables|Default|GetSpringLiquidLocation) (LocalVariables|GetL_CurrentLocation))) 0.0) (/ (Math|Vector|VectorLength (Math|Vector|MakeVector (.x (- (Variables|Default|GetSpringLiquidLocation) (LocalVariables|GetL_CurrentLocation))) (.y (- (Variables|Default|GetSpringLiquidLocation) (LocalVariables|GetL_CurrentLocation))) 0.0)) 5.0)) (Math|Rotator|GetRotationXVector (Class|KismetMathLibrary|QuatRotator _returnvalue_2)) 0.2)))))