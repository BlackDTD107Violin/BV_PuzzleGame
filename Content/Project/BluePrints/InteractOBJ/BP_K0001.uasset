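; BP_K0001 is an interactable key item that can be inspected and used in a keyhole.
; Entering inspection plays an attach sound and hides the mesh; exiting plays a detach sound, then hides the actor and disables its collision.
; An animation switcher handles the keyhole rotation case, currently only a debug print, then optionally detaches the item from the cached player and destroys the actor.
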(event Custom|AnimPlay_RotateInKeyHole
  (Development|PrintString "PlayK0001Anim")
  (if (Variables|Default|GetbDelete%20if%20Complete) ; Detect destroy or not when animation Complete
    (Default|ITEMDetach (Variables|Default|GetPlayer))
    (Actor|DestroyActor)
    (else
      (Development|PrintString "Still in Map and Can Interact"))))

(event EventBeginPlay
  (|CallParentFunction)
  (bind _asbp_first_person_character_tutorial (Utilities|Casting|CastToBP_FirstPersonCharacterTutorial (Game|GetPlayerCharacter 0)))
  (Variables|Default|SetPlayer _asbp_first_person_character_tutorial))

(event EventEnterInspector
  (Audio|SpawnSoundAttached "/Game/Project/Audio/MetaSoundSource/SE/MSS_K0001_Attach.MSS_K0001_Attach" (Variables|Default|GetStaticMesh) "None" "0, 0, 0" "0, 0, 0" "KeepRelativeOffset" false 1.0 1.0 0.0 0 0)
  (Development|SetHiddeninGame (Variables|Default|GetStaticMesh) true false))

(event EventExitInspector
  (Audio|SpawnSoundAttached "/Game/Project/Audio/MetaSoundSource/SE/MSS_K0001_Detach.MSS_K0001_Detach" (Variables|Default|GetStaticMesh) "None" "0, 0, 0" "0, 0, 0" "KeepRelativeOffset" false 1.0 1.0 0.0 0 0)
  (Rendering|SetActorHiddenInGame true)
  (Collision|SetActorEnableCollision false))

(event EventAnimPlaySwitcher
  (params (bDeleteIfComplete :type Boolean) (AnimTarget :type Name :default "None"))
  (Variables|Default|SetbDelete%20if%20Complete bDeleteIfComplete)
  (switch name AnimTarget
    (:RotateInKeyHole
      (CallFunction|AnimPlayRotateinKeyHole))))

(fn ConstructionScript
  (|CallParentFunction))