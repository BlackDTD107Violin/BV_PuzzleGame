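; Nebula cone effect actor with a Nebula particle component, spinning steadily around its local Z axis.
; Tick applies a local rotation scaled by delta time and RotationSpeed.
; BeginPlay enables player input so key 3 sets Time to zero while held and one on release.
; Time feeds only an unconnected AdvanceSimulationByTime call on Nebula, so the key has no visible effect here.
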(event EventBeginPlay
  (Input|EnableInput (Game|GetPlayerController 0)))

(event Collision|EventActorBeginOverlap
  (params (OtherActor :type Actor%20Object%20Reference)))

(event EventTick
  (params (DeltaSeconds :type Float%20%28single-precision%29))
  (Transformation|AddActorLocalRotation (Math|Vector|RotatorfromAxisandAngle "0, 0,1.000000" (* DeltaSeconds (Variables|Default|GetRotation%20Speed))) false false))

(event Input|KeyboardEvents|3
  (params (Key :type Key%20Structure))
  (:Pressed
    (Variables|Default|SetTime 0.0))
  (:Released
    (Variables|Default|SetTime 1.0)))

(fn ConstructionScript)