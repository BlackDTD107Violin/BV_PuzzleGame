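; Test chalice Blueprint that shows on-screen interact and pickup prompts for the player.
; ShowPromptInteract and ShowPromptPick each take a show flag to create and add their prompt widget to the viewport, or remove it.
; A boolean per prompt prevents duplicate widgets on show, while removal runs without checking it.
; The Pickup and Interact events and the construction script are empty stubs.
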(event EventPickup
  (params (InteractTarget :type Actor%20Component%20Object%20Reference)))

(event EventShowPromptInteract
  (params (bIsShow :type Boolean))
  ;[0.05098 0.05098 0.05098] Widget_IO_according to the player is in the Interact Trigger Area or not
  (if bIsShow
    (if (not (Variables|Default|GetbInteractPromptIsExist))
      (bind _returnvalue (UserInterface|CreateWidget "/Game/Developers/LinYanChen/WBP_InteractPrompt.WBP_InteractPrompt_C"))
      (UserInterface|Viewport|AddtoViewport _returnvalue 0)
      (Variables|Default|SetbInteractPromptIsExist true))
    (else
      (Widget|RemovefromParent _returnvalue)
      (Variables|Default|SetbInteractPromptIsExist false))))

(event EventShowPromptPick
  (params (bIsShow :type Boolean))
  ;[0.05098 0.05098 0.05098] Widget_IO_according to the player is in the Pickup Trigger Area or not
  (if bIsShow
    (if (not (Variables|Default|GetbPickPromptIsExist))
      (bind _returnvalue (UserInterface|CreateWidget "/Game/Developers/LinYanChen/WBP_PickPrompt.WBP_PickPrompt_C"))
      (UserInterface|Viewport|AddtoViewport _returnvalue 0)
      (Variables|Default|SetbPickPromptIsExist true))
    (else
      (Widget|RemovefromParent _returnvalue)
      (Variables|Default|SetbPickPromptIsExist false))))

(event EventInteract
  (params (InteractTarget :type Actor%20Component%20Object%20Reference)))

(fn ConstructionScript)